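; BP_BulletCase is an ejected shell casing effect that flies by projectile movement with rotation and destroys itself after three seconds.
; On spawn, a timeline scales its sphere up from a small size.
; Each bounce plays a shell-drop sound, and the first stops the spin and, after a brief delay, switches the sphere to physics simulation.
; Later sphere hits replay the sound, throttled by a resetting DoOnce.
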(event `self.ReceiveBeginPlay`
  (`|ExecutionSequence`
    (:`then_0`
      (`KismetSystemLibrary.Delay` 3.0)
      (`self.K2_DestroyActor`))
    (:`then_1`
      (bind (_direction _newtrack_0) (`Timeline|Timeline_0` :!via `PlayFromStart`)
        (:`Update`
          (`SceneComponent.SetRelativeScale3D` (`self.Sphere`) (`KismetMathLibrary.VLerp` (0.2 0.2 0.2) (0.7 0.7 0.7) _newtrack_0)))))))

(event `self.Sphere.OnComponentHit`
  (params (HitComponent :type "PrimitiveComponent Object Reference") (OtherActor :type "Actor Object Reference") (OtherComp :type "PrimitiveComponent Object Reference") (NormalImpulse :type "Vector Structure") (Hit :type "HitResult Structure (by ref)"))
  (`/Engine/EditorBlueprintResources/StandardMacros.DoOnce` false :!label _label
    (:`Completed`
      (`GameplayStatics.PlaySoundAtLocation` "/Game/AUDIO/SFX_Weapons/SC_ShellDrop.SC_ShellDrop" (`self.K2_GetActorLocation`) (struct) 1.0 1.0 0.0 "/Game/kosm_fps_assets/Misc/SoundFX/SoundAttenuationLow.SoundAttenuationLow" null null)
      (`KismetSystemLibrary.Delay` 0.4)
      (goto _label :!via `Reset`))))

(event `self.ProjectileMovement.OnProjectileBounce`
  (params (ImpactResult :type "HitResult Structure (by ref)") (ImpactVelocity :type "Vector Structure (by ref)"))
  (`GameplayStatics.PlaySoundAtLocation` "/Game/AUDIO/SFX_Weapons/SC_ShellDrop.SC_ShellDrop" (`self.K2_GetActorLocation`) (struct) 1.0 1.0 0.0 "/Game/kosm_fps_assets/Misc/SoundFX/SoundAttenuationLow.SoundAttenuationLow" null null)
  (`/Engine/EditorBlueprintResources/StandardMacros.DoOnce` false
    (:`Completed`
      (set `RotatingMovementComponent.RotationRate` (struct) (`self.RotatingMovement`))
      (`KismetSystemLibrary.Delay` 0.1)
      (`PrimitiveComponent.SetSimulatePhysics` (`self.Sphere`) true))))

(fn `UserConstructionScript`)