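; Episode 6 cinematic dialogue bank that shows infolink cutscene lines for boss fights, island, lab, tower and docks scenes, the chief intro, and an ending.
; Each scene event switches on a Line index, creating a BP_infolink_cutscene widget with portrait, speaker and hardcoded text; only the TOWER2 lines are unskippable.
; Quit restores the player HUD and removes those widgets.
; Extras include a hacker music cue and clearing an equipment-log popup at the docks.
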(event `CEO bossfight`
  (params (Line :type Integer :default 1))
  (switch `int` Line
    (:`0`
      (bind _returnvalue (`|CreateWidget` "/Game/VN_UI/BP_infolink_cutscene.BP_infolink_cutscene_C")) ; 0
      (`UserWidget.AddToViewport` _returnvalue 0)
      (`/Game/VN_UI/BP_infolink_cutscene.MESSAGE` _returnvalue "/Game/VN_UI/Avatars/T_Infolink_CEO.T_Infolink_CEO" "Let's end this farce" "CEO"))
    (:`1`
      (bind _returnvalue_2 (`|CreateWidget` "/Game/VN_UI/BP_infolink_cutscene.BP_infolink_cutscene_C")) ; 1
      (`UserWidget.AddToViewport` _returnvalue_2 0)
      (`/Game/VN_UI/BP_infolink_cutscene.MESSAGE` _returnvalue_2 "/Game/VN_UI/Avatars/T_Infolink_CEO.T_Infolink_CEO" "Bring it on!" "CEO"))))

(event `CTF1_Hackmusic`
  (`GameplayStatics.SpawnSound2D` "/Game/MISSIONS/EP3/Music/SC_CTF1_Hacker.SC_CTF1_Hacker" 0.7 1.0 0.0 null))

(event `Quit`
  (bind _player (`/Game/Blueprints/NewFunctionLibrary.get player`))
  (`Widget.SetVisibility` (`/Game/Blueprints/CHARACTERS/fpsMovementCharacter_light_1_vq3.HUD` _player) "Visible")
  (bind _foundwidgets (`WidgetBlueprintLibrary.GetAllWidgetsOfClass` "/Game/VN_UI/BP_infolink_cutscene.BP_infolink_cutscene_C"))
  (`Widget.RemoveFromParent` _foundwidgets))

(event `Dialogue Lab helsing`
  (params (Line :type Integer :default 1))
  (switch `int` Line
    (:`0`
      (bind _returnvalue (`|CreateWidget` "/Game/VN_UI/BP_infolink_cutscene.BP_infolink_cutscene_C"))
      (`UserWidget.AddToViewport` _returnvalue 0)
      (`/Game/VN_UI/BP_infolink_cutscene.MESSAGE` _returnvalue "/Game/VN_UI/Avatars/T_Infolink_Molly.T_Infolink_Molly" "Ok. We’re fucked. I’m fucked!" "Molly"))
    (:`1`
      (bind _returnvalue_2 (`|CreateWidget` "/Game/VN_UI/BP_infolink_cutscene.BP_infolink_cutscene_C"))
      (`UserWidget.AddToViewport` _returnvalue_2 0)
      (`/Game/VN_UI/BP_infolink_cutscene.MESSAGE` _returnvalue_2 "/Game/VN_UI/Avatars/T_Infolink_Hacker.T_Infolink_Hacker" "He’s not there? I suspected as much." "Hacker"))
    (:`2`
      (bind _returnvalue_3 (`|CreateWidget` "/Game/VN_UI/BP_infolink_cutscene.BP_infolink_cutscene_C"))
      (`UserWidget.AddToViewport` _returnvalue_3 0)
      (`/Game/VN_UI/BP_infolink_cutscene.MESSAGE` _returnvalue_3 "/Game/VN_UI/Avatars/T_Infolink_Molly.T_Infolink_Molly" "Well, why didn’t you tell me? The hell am I going to do now? I’m at the bottom of a black site in the tropics, I can’t just pop out to the beach like nothing happened!" "Molly"))
    (:`3`
      (bind _returnvalue_4 (`|CreateWidget` "/Game/VN_UI/BP_infolink_cutscene.BP_infolink_cutscene_C"))
      (`UserWidget.AddToViewport` _returnvalue_4 0)
      (`/Game/VN_UI/BP_infolink_cutscene.MESSAGE` _returnvalue_4 "/Game/VN_UI/Avatars/T_Infolink_Hacker.T_Infolink_Hacker" "That might be the best thing to do right now. We have time for a quick exfil. \nUnfortunately I tripped a silent alarm. You have tangos incoming. \nBUT! I did find something interesting in one of the armories." "Hacker"))
    (:`4`
      (bind _returnvalue_5 (`|CreateWidget` "/Game/VN_UI/BP_infolink_cutscene.BP_infolink_cutscene_C"))
      (`UserWidget.AddToViewport` _returnvalue_5 0)
      (`/Game/VN_UI/BP_infolink_cutscene.MESSAGE` _returnvalue_5 "/Game/VN_UI/Avatars/T_Infolink_Hacker.T_Infolink_Hacker" "Going dark now, see you topside." "Hacker"))
    (:`5`
      (bind _returnvalue_6 (`|CreateWidget` "/Game/VN_UI/BP_infolink_cutscene.BP_infolink_cutscene_C"))
      (`UserWidget.AddToViewport` _returnvalue_6 0)
      (`/Game/VN_UI/BP_infolink_cutscene.MESSAGE` _returnvalue_6 "/Game/VN_UI/Avatars/T_Infolink_Hacker.T_Infolink_Hacker" "That might be the best thing to do right now. We have time for a quick exfil. \nUnfortunately I tripped a silent alarm. You have tangos incoming. \nTry to stay to alive. Going dark now, good luck." "Hacker"))))

(event `TOWER2`
  (params (Line :type Integer :default 1))
  (switch `int` Line
    (:`0`
      (bind _returnvalue (`|CreateWidget` "/Game/VN_UI/BP_infolink_cutscene.BP_infolink_cutscene_C" null false))
      (`UserWidget.AddToViewport` _returnvalue 0)
      (`/Game/VN_UI/BP_infolink_cutscene.MESSAGE` _returnvalue "/Game/VN_UI/Avatars/Arcade_avatars/T_Arc_Major.T_Arc_Major" "Alright gang, this is where we split up. We'll go ahead and search this wing, keep in touch via comms!" "Major"))
    (:`1`
      (bind _returnvalue_2 (`|CreateWidget` "/Game/VN_UI/BP_infolink_cutscene.BP_infolink_cutscene_C" null false))
      (`UserWidget.AddToViewport` _returnvalue_2 0)
      (`/Game/VN_UI/BP_infolink_cutscene.MESSAGE` _returnvalue_2 "/Game/VN_UI/Avatars/Arcade_avatars/T_Arc_Molly.T_Arc_Molly" "What the...?" "Molly"))
    (:`2`
      (bind _returnvalue_3 (`|CreateWidget` "/Game/VN_UI/BP_infolink_cutscene.BP_infolink_cutscene_C" null false))
      (`UserWidget.AddToViewport` _returnvalue_3 0)
      (`/Game/VN_UI/BP_infolink_cutscene.MESSAGE` _returnvalue_3 "/Game/VN_UI/Avatars/Arcade_avatars/T_Arc_Major.T_Arc_Major" "Crap, are we too late? What happened?" "Major "))
    (:`3`
      (bind _returnvalue_4 (`|CreateWidget` "/Game/VN_UI/BP_infolink_cutscene.BP_infolink_cutscene_C" null false))
      (`UserWidget.AddToViewport` _returnvalue_4 0)
      (`/Game/VN_UI/BP_infolink_cutscene.MESSAGE` _returnvalue_4 "/Game/VN_UI/Avatars/Arcade_avatars/T_Arc_Molly.T_Arc_Molly" "Something terrible. We must go, now." "Molly"))
    (:`4`
      (bind _returnvalue_5 (`|CreateWidget` "/Game/VN_UI/BP_infolink_cutscene.BP_infolink_cutscene_C" null false))
      (`UserWidget.AddToViewport` _returnvalue_5 0)
      (`/Game/VN_UI/BP_infolink_cutscene.MESSAGE` _returnvalue_5 "/Game/VN_UI/Avatars/T_Infolink_Hacker.T_Infolink_Hacker" "Can confirm, reality's being held at the seems here. We've got an hour tops before the whole place unfolds." "Hacker "))
    (:`5`
      (bind _returnvalue_6 (`|CreateWidget` "/Game/VN_UI/BP_infolink_cutscene.BP_infolink_cutscene_C" null false))
      (`UserWidget.AddToViewport` _returnvalue_6 0)
      (`/Game/VN_UI/BP_infolink_cutscene.MESSAGE` _returnvalue_6 "/Game/VN_UI/Avatars/Arcade_avatars/T_Arc_Molly.T_Arc_Molly" "You heard him, let's get moving." "Molly"))))

(event `Helsing boss fight`
  (params (Line :type Integer :default 1))
  (switch `int` Line
    (:`0`
      (bind _returnvalue (`|CreateWidget` "/Game/VN_UI/BP_infolink_cutscene.BP_infolink_cutscene_C")) ; 0
      (`UserWidget.AddToViewport` _returnvalue 0)
      (`/Game/VN_UI/BP_infolink_cutscene.MESSAGE` _returnvalue "/Game/VN_UI/Avatars/T_Infolink_Helsing.T_Infolink_Helsing" "Were you looking for this?" "Helsing"))
    (:`1`
      (bind _returnvalue_2 (`|CreateWidget` "/Game/VN_UI/BP_infolink_cutscene.BP_infolink_cutscene_C"))
      (`UserWidget.AddToViewport` _returnvalue_2 0)
      (`/Game/VN_UI/BP_infolink_cutscene.MESSAGE` _returnvalue_2 "/Game/VN_UI/Avatars/T_Infolink_Molly.T_Infolink_Molly" "What are YOU doing here?!" "Molly"))
    (:`2`
      (bind _returnvalue_3 (`|CreateWidget` "/Game/VN_UI/BP_infolink_cutscene.BP_infolink_cutscene_C"))
      (`UserWidget.AddToViewport` _returnvalue_3 0)
      (`/Game/VN_UI/BP_infolink_cutscene.MESSAGE` _returnvalue_3 "/Game/VN_UI/Avatars/T_Infolink_Helsing.T_Infolink_Helsing" "Lucky for me, the Wizard’s ritual was indeed pretty shoddy: my memories came back. I clearly see what I have to do…again." "Helsing"))
    (:`3`
      (bind _returnvalue_4 (`|CreateWidget` "/Game/VN_UI/BP_infolink_cutscene.BP_infolink_cutscene_C"))
      (`UserWidget.AddToViewport` _returnvalue_4 0)
      (`/Game/VN_UI/BP_infolink_cutscene.MESSAGE` _returnvalue_4 "/Game/VN_UI/Avatars/T_Infolink_Molly.T_Infolink_Molly" "“Again”? You…You are the hunter!" "Molly"))
    (:`4`
      (bind _returnvalue_5 (`|CreateWidget` "/Game/VN_UI/BP_infolink_cutscene.BP_infolink_cutscene_C"))
      (`UserWidget.AddToViewport` _returnvalue_5 0)
      (`/Game/VN_UI/BP_infolink_cutscene.MESSAGE` _returnvalue_5 "/Game/VN_UI/Avatars/T_Infolink_Helsing.T_Infolink_Helsing" "I can’t let your ilk walk the earth as if nothing happened." "Helsing"))
    (:`5`
      (bind _returnvalue_6 (`|CreateWidget` "/Game/VN_UI/BP_infolink_cutscene.BP_infolink_cutscene_C"))
      (`UserWidget.AddToViewport` _returnvalue_6 0)
      (`/Game/VN_UI/BP_infolink_cutscene.MESSAGE` _returnvalue_6 "/Game/VN_UI/Avatars/T_Infolink_Molly.T_Infolink_Molly" "Banishing us all won’t solve the issue!" "Molly"))
    (:`6`
      (bind _returnvalue_7 (`|CreateWidget` "/Game/VN_UI/BP_infolink_cutscene.BP_infolink_cutscene_C"))
      (`UserWidget.AddToViewport` _returnvalue_7 0)
      (`/Game/VN_UI/BP_infolink_cutscene.MESSAGE` _returnvalue_7 "/Game/VN_UI/Avatars/T_Infolink_Helsing.T_Infolink_Helsing" "You leave me no choice, then." "Helsing"))
    (:`7`
      (bind _returnvalue_8 (`|CreateWidget` "/Game/VN_UI/BP_infolink_cutscene.BP_infolink_cutscene_C"))
      (`UserWidget.AddToViewport` _returnvalue_8 0)
      (`/Game/VN_UI/BP_infolink_cutscene.MESSAGE` _returnvalue_8 "/Game/VN_UI/Avatars/T_Infolink_Molly.T_Infolink_Molly" " I’m sorry Helsing, but you're not the hero of this story..." "Molly"))
    (:`8`
      (bind _returnvalue_9 (`|CreateWidget` "/Game/VN_UI/BP_infolink_cutscene.BP_infolink_cutscene_C"))
      (`UserWidget.AddToViewport` _returnvalue_9 0)
      (`/Game/VN_UI/BP_infolink_cutscene.MESSAGE` _returnvalue_9 "/Game/VN_UI/Avatars/T_Infolink_Helsing.T_Infolink_Helsing" "Then set me free." "Helsing"))))

(event `Dialogue Island Gmax discovery`
  (params (Line :type Integer :default 1))
  ;[1 1 1] CTF3 Gmax discovery
  (switch `int` Line
    (:`0`
      (bind _returnvalue (`|CreateWidget` "/Game/VN_UI/BP_infolink_cutscene.BP_infolink_cutscene_C")) ; 0
      (`UserWidget.AddToViewport` _returnvalue 0)
      (`/Game/VN_UI/BP_infolink_cutscene.MESSAGE` _returnvalue "/Game/VN_UI/Avatars/T_Infolink_Hacker.T_Infolink_Hacker" "Hold it, don’t go any further!" "Hacker"))
    (:`1`
      (bind _returnvalue_2 (`|CreateWidget` "/Game/VN_UI/BP_infolink_cutscene.BP_infolink_cutscene_C"))
      (`UserWidget.AddToViewport` _returnvalue_2 0)
      (`/Game/VN_UI/BP_infolink_cutscene.MESSAGE` _returnvalue_2 "/Game/VN_UI/Avatars/T_Infolink_Molly.T_Infolink_Molly" "Did not plan to. This place looks like trouble." "Molly"))
    (:`2`
      (bind _returnvalue_3 (`|CreateWidget` "/Game/VN_UI/BP_infolink_cutscene.BP_infolink_cutscene_C"))
      (`UserWidget.AddToViewport` _returnvalue_3 0)
      (`/Game/VN_UI/BP_infolink_cutscene.MESSAGE` _returnvalue_3 "/Game/VN_UI/Avatars/T_Infolink_Hacker.T_Infolink_Hacker" "Yes, this is a covert Galactamax facility." "Hacker"))
    (:`3`
      (bind _returnvalue_4 (`|CreateWidget` "/Game/VN_UI/BP_infolink_cutscene.BP_infolink_cutscene_C"))
      (`UserWidget.AddToViewport` _returnvalue_4 0)
      (`/Game/VN_UI/BP_infolink_cutscene.MESSAGE` _returnvalue_4 "/Game/VN_UI/Avatars/T_Infolink_Molly.T_Infolink_Molly" "What? Like, the billion-dollar corp? The one that started blood sports entertainment?" "Molly"))
    (:`4`
      (bind _returnvalue_5 (`|CreateWidget` "/Game/VN_UI/BP_infolink_cutscene.BP_infolink_cutscene_C"))
      (`UserWidget.AddToViewport` _returnvalue_5 0)
      (`/Game/VN_UI/BP_infolink_cutscene.MESSAGE` _returnvalue_5 "/Game/VN_UI/Avatars/T_Infolink_Hacker.T_Infolink_Hacker" "Yeah, but the name was different back then. And they had a show…" "Hacker"))
    (:`5`
      (bind _returnvalue_6 (`|CreateWidget` "/Game/VN_UI/BP_infolink_cutscene.BP_infolink_cutscene_C"))
      (`UserWidget.AddToViewport` _returnvalue_6 0)
      (`/Game/VN_UI/BP_infolink_cutscene.MESSAGE` _returnvalue_6 "/Game/VN_UI/Avatars/T_Infolink_Molly.T_Infolink_Molly" "I remember! \"Death Game”. I think one of my cousins was a fan – convicts shooting each other with stupidly big guns.  \nCan’t believe this was on the TV. It ran for a few years, right? And then it got banned." "Molly"))
    (:`6`
      (bind _returnvalue_7 (`|CreateWidget` "/Game/VN_UI/BP_infolink_cutscene.BP_infolink_cutscene_C"))
      (`UserWidget.AddToViewport` _returnvalue_7 0)
      (`/Game/VN_UI/BP_infolink_cutscene.MESSAGE` _returnvalue_7 "/Game/VN_UI/Avatars/T_Infolink_Hacker.T_Infolink_Hacker" "Bingo. It was outlawed with the Lieb/Kohn Act. The company stayed afloat though – and became Galactamax. And they could afford black sites, like this one. \nI don’t think we can handle that, there are a lot of heat signatures there, including non-human. Let’s go get that flag instead." "Hacker"))))

(event `Dialogue island part 2_1`
  (params (Line :type Integer :default 1))
  ;[1 1 1] CTF3 Part 2 -1
  (switch `int` Line
    (:`0`
      (bind _returnvalue (`|CreateWidget` "/Game/VN_UI/BP_infolink_cutscene.BP_infolink_cutscene_C")) ; 0
      (`UserWidget.AddToViewport` _returnvalue 0)
      (`/Game/VN_UI/BP_infolink_cutscene.MESSAGE` _returnvalue "/Game/VN_UI/Avatars/T_Infolink_Hacker.T_Infolink_Hacker" "Shit, they’re here. Stay low." "Hacker"))
    (:`1`
      (bind _returnvalue_2 (`|CreateWidget` "/Game/VN_UI/BP_infolink_cutscene.BP_infolink_cutscene_C"))
      (`UserWidget.AddToViewport` _returnvalue_2 0)
      (`/Game/VN_UI/BP_infolink_cutscene.MESSAGE` _returnvalue_2 "/Game/VN_UI/Avatars/T_Infolink_Galactamax.T_Infolink_Galactamax" "Control, Spear 48: Perimeter breach. Executing full response." "R-Frame"))
    (:`2`
      (bind _returnvalue_3 (`|CreateWidget` "/Game/VN_UI/BP_infolink_cutscene.BP_infolink_cutscene_C"))
      (`UserWidget.AddToViewport` _returnvalue_3 0)
      (`/Game/VN_UI/BP_infolink_cutscene.MESSAGE` _returnvalue_3 "/Game/VN_UI/Avatars/T_Infolink_MajorCommando.T_Infolink_MajorCommando" "Woah, we’re just standing here!" "Major"))
    (:`3`
      (bind _returnvalue_4 (`|CreateWidget` "/Game/VN_UI/BP_infolink_cutscene.BP_infolink_cutscene_C"))
      (`UserWidget.AddToViewport` _returnvalue_4 0)
      (`/Game/VN_UI/BP_infolink_cutscene.MESSAGE` _returnvalue_4 "/Game/VN_UI/Avatars/T_Infolink_Wizard.T_Infolink_Wizard" "Enough! I’m getting us outta here!" "Wizard"))
    (:`4`
      (bind _returnvalue_5 (`|CreateWidget` "/Game/VN_UI/BP_infolink_cutscene.BP_infolink_cutscene_C"))
      (`UserWidget.AddToViewport` _returnvalue_5 0)
      (`/Game/VN_UI/BP_infolink_cutscene.MESSAGE` _returnvalue_5 "/Game/VN_UI/Avatars/T_Infolink_Rumbletron.T_Infolink_Rumbletron" "Wait! What about [Molly, Molly, Mo-] and the [Vampire Savior]?" "Rumbletron"))
    (:`5`
      (bind _returnvalue_6 (`|CreateWidget` "/Game/VN_UI/BP_infolink_cutscene.BP_infolink_cutscene_C"))
      (`UserWidget.AddToViewport` _returnvalue_6 0)
      (`/Game/VN_UI/BP_infolink_cutscene.MESSAGE` _returnvalue_6 "/Game/VN_UI/Avatars/T_Infolink_Galactamax.T_Infolink_Galactamax" "Target lost. Sweep and resume." "R-Frame"))
    (:`6`
      (bind _returnvalue_7 (`|CreateWidget` "/Game/VN_UI/BP_infolink_cutscene.BP_infolink_cutscene_C"))
      (`UserWidget.AddToViewport` _returnvalue_7 0)
      (`/Game/VN_UI/BP_infolink_cutscene.MESSAGE` _returnvalue_7 "/Game/VN_UI/Avatars/T_Infolink_Hacker.T_Infolink_Hacker" "Hide, quick! And don’t move!" "Hacker"))))

(event `Dialogues Chief intro`
  (params (Line :type Integer :default 1))
  (switch `int` Line
    (:`0`
      ;[1 1 1] VILLAGE CHIEF INTRO
      (bind _returnvalue (`|CreateWidget` "/Game/VN_UI/BP_infolink_cutscene.BP_infolink_cutscene_C")) ; 0
      (`UserWidget.AddToViewport` _returnvalue 0)
      (`/Game/VN_UI/BP_infolink_cutscene.MESSAGE` _returnvalue "/Game/VN_UI/Avatars/T_Infolink_ChiefNative.T_Infolink_ChiefNative" "So, you must be the lost soul that has been causing all this racket. Welcome to my village, our mutual friend has already told me everything: you're looking for a way out of here, aren't you?" "Chief"))
    (:`1`
      (bind _returnvalue_2 (`|CreateWidget` "/Game/VN_UI/BP_infolink_cutscene.BP_infolink_cutscene_C"))
      (`UserWidget.AddToViewport` _returnvalue_2 0)
      (`/Game/VN_UI/BP_infolink_cutscene.MESSAGE` _returnvalue_2 "/Game/VN_UI/Avatars/T_Infolink_Molly.T_Infolink_Molly" "Indeed, could you help me out with that?" "Molly"))
    (:`2`
      (bind _returnvalue_3 (`|CreateWidget` "/Game/VN_UI/BP_infolink_cutscene.BP_infolink_cutscene_C"))
      (`UserWidget.AddToViewport` _returnvalue_3 0)
      (`/Game/VN_UI/BP_infolink_cutscene.MESSAGE` _returnvalue_3 "/Game/VN_UI/Avatars/T_Infolink_ChiefNative.T_Infolink_ChiefNative" "Absolutely. Creating a passage to your final destination should be possible, but I'll need you to gather your companions before we can go through with it: I don't think I'd be able to open more than one in such a short notice." "Chief"))
    (:`3`
      (bind _returnvalue_4 (`|CreateWidget` "/Game/VN_UI/BP_infolink_cutscene.BP_infolink_cutscene_C"))
      (`UserWidget.AddToViewport` _returnvalue_4 0)
      (`/Game/VN_UI/BP_infolink_cutscene.MESSAGE` _returnvalue_4 "/Game/VN_UI/Avatars/T_Infolink_Molly.T_Infolink_Molly" "I'll just go pick'em up while you do your preparations, if you tell me where I should start looking." "Molly"))
    (:`4`
      (bind _returnvalue_5 (`|CreateWidget` "/Game/VN_UI/BP_infolink_cutscene.BP_infolink_cutscene_C"))
      (`UserWidget.AddToViewport` _returnvalue_5 0)
      (`/Game/VN_UI/BP_infolink_cutscene.MESSAGE` _returnvalue_5 "/Game/VN_UI/Avatars/T_Infolink_ChiefNative.T_Infolink_ChiefNative" "Ah yes, your \"Hacker\" friend did bring that up. They're currently held captive in a Galactamax facility, locked inside a virtual dimension isolated from the rest of Galactamax's network. If you stole the physical drive containing it and brought it here, me and our \"Hacker\" friend could devise a way to extract them from it." "Chief"))
    (:`5`
      (bind _returnvalue_6 (`|CreateWidget` "/Game/VN_UI/BP_infolink_cutscene.BP_infolink_cutscene_C"))
      (`UserWidget.AddToViewport` _returnvalue_6 0)
      (`/Game/VN_UI/BP_infolink_cutscene.MESSAGE` _returnvalue_6 "/Game/VN_UI/Avatars/T_Infolink_Molly.T_Infolink_Molly" "Sounds good,  how do I get there?" "Molly"))
    (:`6`
      (bind _returnvalue_7 (`|CreateWidget` "/Game/VN_UI/BP_infolink_cutscene.BP_infolink_cutscene_C"))
      (`UserWidget.AddToViewport` _returnvalue_7 0)
      (`/Game/VN_UI/BP_infolink_cutscene.MESSAGE` _returnvalue_7 "/Game/VN_UI/Avatars/T_Infolink_ChiefNative.T_Infolink_ChiefNative" "Back when they first came here, the Galactamax researchers stumbled into our tunnel network while digging their own. They thought they had closed the passage after that, but we dug a secondary one just in case: you should be able to access it by going back to the catacombs whence you came and looking for a tunnel blocked by a guard. I'll tell him to let you through right away." "Chief"))
    (:`7`
      (bind _returnvalue_8 (`|CreateWidget` "/Game/VN_UI/BP_infolink_cutscene.BP_infolink_cutscene_C"))
      (`UserWidget.AddToViewport` _returnvalue_8 0)
      (`/Game/VN_UI/BP_infolink_cutscene.MESSAGE` _returnvalue_8 "/Game/VN_UI/Avatars/T_Infolink_Molly.T_Infolink_Molly" "Thank you." "Molly"))
    (:`8`
      (bind _returnvalue_9 (`|CreateWidget` "/Game/VN_UI/BP_infolink_cutscene.BP_infolink_cutscene_C"))
      (`UserWidget.AddToViewport` _returnvalue_9 0)
      (`/Game/VN_UI/BP_infolink_cutscene.MESSAGE` _returnvalue_9 "/Game/VN_UI/Avatars/T_Infolink_ChiefNative.T_Infolink_ChiefNative" "Good hunting." "Chief"))))

(event `CEO cutscene`
  (params (Line :type Integer :default 1))
  (switch `int` Line
    (:`0`
      ;[1 1 1] CEO dialogue before final bossfight.
      ; His lines are left deliberately vague so that
      ;  they can apply to both Molly or Newcat reaching the office.
      (bind _returnvalue (`|CreateWidget` "/Game/VN_UI/BP_infolink_cutscene.BP_infolink_cutscene_C"))
      (`UserWidget.AddToViewport` _returnvalue 0)
      (`/Game/VN_UI/BP_infolink_cutscene.MESSAGE` _returnvalue "/Game/VN_UI/Avatars/T_Infolink_CEO.T_Infolink_CEO" "You made it all the way up here." "CEO"))
    (:`1`
      (bind _returnvalue_2 (`|CreateWidget` "/Game/VN_UI/BP_infolink_cutscene.BP_infolink_cutscene_C"))
      (`UserWidget.AddToViewport` _returnvalue_2 0)
      (`/Game/VN_UI/BP_infolink_cutscene.MESSAGE` _returnvalue_2 "/Game/VN_UI/Avatars/T_Infolink_CEO.T_Infolink_CEO" "Fine, it is time to end this charade in an honorable way." "CEO"))
    (:`2`
      (bind _returnvalue_3 (`|CreateWidget` "/Game/VN_UI/BP_infolink_cutscene.BP_infolink_cutscene_C"))
      (`UserWidget.AddToViewport` _returnvalue_3 0)
      (`/Game/VN_UI/BP_infolink_cutscene.MESSAGE` _returnvalue_3 "/Game/VN_UI/Avatars/T_Infolink_CEO.T_Infolink_CEO" "Meet me on the rooftop, I'll be waiting for you." "CEO"))))

(event `DOCKS`
  (params (Line :type Integer :default 1))
  (switch `int` Line
    (:`0`
      (bind _returnvalue (`|CreateWidget` "/Game/VN_UI/BP_infolink_cutscene.BP_infolink_cutscene_C")) ; 0
      (`UserWidget.AddToViewport` _returnvalue 0)
      (`/Game/VN_UI/BP_infolink_cutscene.MESSAGE` _returnvalue "/Game/VN_UI/Avatars/T_Infolink_MajorCommando.T_Infolink_MajorCommando" "Ah, it's good to be back in the US of A! What now, though?" "Major")
      (bind _foundwidgets (`WidgetBlueprintLibrary.GetAllWidgetsOfClass` "/Game/Blueprints/UI/UI_PauseTutorials/W_PauseTutorialGeneric_small_noinputs_EquiptmentLog.W_PauseTutorialGeneric_small_noinputs_EquiptmentLog_C" false))
      (`Widget.RemoveFromParent` _foundwidgets))
    (:`1`
      (bind _returnvalue_2 (`|CreateWidget` "/Game/VN_UI/BP_infolink_cutscene.BP_infolink_cutscene_C"))
      (`UserWidget.AddToViewport` _returnvalue_2 0)
      (`/Game/VN_UI/BP_infolink_cutscene.MESSAGE` _returnvalue_2 "/Game/VN_UI/Avatars/T_Infolink_Hacker.T_Infolink_Hacker" "Now we hit GMax directly." "Hacker"))
    (:`2`
      (bind _returnvalue_3 (`|CreateWidget` "/Game/VN_UI/BP_infolink_cutscene.BP_infolink_cutscene_C")) ; 2
      (`UserWidget.AddToViewport` _returnvalue_3 0)
      (`/Game/VN_UI/BP_infolink_cutscene.MESSAGE` _returnvalue_3 "/Game/VN_UI/Avatars/T_Infolink_Hacker.T_Infolink_Hacker" "Across from that warehouse you'll find a private train line connecting these docks to their HQ, It's our quickest way in." "Hacker"))
    (:`3`
      (bind _returnvalue_4 (`|CreateWidget` "/Game/VN_UI/BP_infolink_cutscene.BP_infolink_cutscene_C"))
      (`UserWidget.AddToViewport` _returnvalue_4 0)
      (`/Game/VN_UI/BP_infolink_cutscene.MESSAGE` _returnvalue_4 "/Game/VN_UI/Avatars/T_Infolink_Hacker.T_Infolink_Hacker" "The gates are opened from the inside, and it looks like you can reach the other side by going through that cargo ship." "Hacker"))
    (:`4`
      (bind _returnvalue_5 (`|CreateWidget` "/Game/VN_UI/BP_infolink_cutscene.BP_infolink_cutscene_C"))
      (`UserWidget.AddToViewport` _returnvalue_5 0)
      (`/Game/VN_UI/BP_infolink_cutscene.MESSAGE` _returnvalue_5 "/Game/VN_UI/Avatars/T_Infolink_Hacker.T_Infolink_Hacker" "Looks like your friends were disarmed; you'll need to clear the area on your own before they can follow you in." "Hacker"))
    (:`5`
      (bind _returnvalue_6 (`|CreateWidget` "/Game/VN_UI/BP_infolink_cutscene.BP_infolink_cutscene_C"))
      (`UserWidget.AddToViewport` _returnvalue_6 0)
      (`/Game/VN_UI/BP_infolink_cutscene.MESSAGE` _returnvalue_6 "/Game/VN_UI/Avatars/T_Infolink_Molly.T_Infolink_Molly" "Coast is clear, you can come out now." "Molly"))
    (:`6`
      (bind _returnvalue_7 (`|CreateWidget` "/Game/VN_UI/BP_infolink_cutscene.BP_infolink_cutscene_C"))
      (`UserWidget.AddToViewport` _returnvalue_7 0)
      (`/Game/VN_UI/BP_infolink_cutscene.MESSAGE` _returnvalue_7 "/Game/VN_UI/Avatars/T_Infolink_Molly.T_Infolink_Molly" "Gonna go ahead and clear the rest of'em, you sit tight and wait for me, alright?" "Molly"))
    (:`7`
      (bind _returnvalue_8 (`|CreateWidget` "/Game/VN_UI/BP_infolink_cutscene.BP_infolink_cutscene_C"))
      (`UserWidget.AddToViewport` _returnvalue_8 0)
      (`/Game/VN_UI/BP_infolink_cutscene.MESSAGE` _returnvalue_8 "/Game/VN_UI/Avatars/T_Infolink_Hacker.T_Infolink_Hacker" "Here's your ride, open the gate at the end of that corridor and you can all get out of here." "Hacker"))
    (:`8`
      (bind _returnvalue_9 (`|CreateWidget` "/Game/VN_UI/BP_infolink_cutscene.BP_infolink_cutscene_C"))
      (`UserWidget.AddToViewport` _returnvalue_9 0)
      (`/Game/VN_UI/BP_infolink_cutscene.MESSAGE` _returnvalue_9 "/Game/VN_UI/Avatars/T_Infolink_MajorCommando.T_Infolink_MajorCommando" "Aye, excellent work! Major's leaving the building!" "Major"))))

(event `Dialogue island hacker mid`
  (params (Line :type Integer :default 1))
  (switch `int` Line
    (:`0`
      (bind _returnvalue (`|CreateWidget` "/Game/VN_UI/BP_infolink_cutscene.BP_infolink_cutscene_C"))
      (`UserWidget.AddToViewport` _returnvalue 0)
      (`/Game/VN_UI/BP_infolink_cutscene.MESSAGE` _returnvalue "/Game/VN_UI/Avatars/T_Infolink_Molly.T_Infolink_Molly" "Oh, it’s you." "Molly"))
    (:`1`
      (bind _returnvalue_2 (`|CreateWidget` "/Game/VN_UI/BP_infolink_cutscene.BP_infolink_cutscene_C"))
      (`UserWidget.AddToViewport` _returnvalue_2 0)
      (`/Game/VN_UI/BP_infolink_cutscene.MESSAGE` _returnvalue_2 "/Game/VN_UI/Avatars/T_Infolink_Hacker.T_Infolink_Hacker" " Yes. I bring dire news. This is the worst Rupture Event recorded in decades. And you?" "Hacker"))
    (:`2`
      (bind _returnvalue_3 (`|CreateWidget` "/Game/VN_UI/BP_infolink_cutscene.BP_infolink_cutscene_C"))
      (`UserWidget.AddToViewport` _returnvalue_3 0)
      (`/Game/VN_UI/BP_infolink_cutscene.MESSAGE` _returnvalue_3 "/Game/VN_UI/Avatars/T_Infolink_Molly.T_Infolink_Molly" "I have to get the blue flag – why, I don’t know. But maybe it will help us stitch the realities together. \nAt least that’s what the Wizard is thinking." "Molly"))
    (:`3`
      (bind _returnvalue_4 (`|CreateWidget` "/Game/VN_UI/BP_infolink_cutscene.BP_infolink_cutscene_C"))
      (`UserWidget.AddToViewport` _returnvalue_4 0)
      (`/Game/VN_UI/BP_infolink_cutscene.MESSAGE` _returnvalue_4 "/Game/VN_UI/Avatars/T_Infolink_Hacker.T_Infolink_Hacker" "Ok. Just watch your back. This island is not as deserted as your friend, the Wiz thought. People here… are very distrustful to outsiders. \nAnd they have been hunting undead for centuries." "Hacker"))
    (:`4`
      (bind _returnvalue_5 (`|CreateWidget` "/Game/VN_UI/BP_infolink_cutscene.BP_infolink_cutscene_C"))
      (`UserWidget.AddToViewport` _returnvalue_5 0)
      (`/Game/VN_UI/BP_infolink_cutscene.MESSAGE` _returnvalue_5 "/Game/VN_UI/Avatars/T_Infolink_Hacker.T_Infolink_Hacker" "They have perfected the weapons that just… erase the soul. Just try to stay out of sight." "Hacker"))
    (:`5`
      (bind _returnvalue_6 (`|CreateWidget` "/Game/VN_UI/BP_infolink_cutscene.BP_infolink_cutscene_C"))
      (`UserWidget.AddToViewport` _returnvalue_6 0)
      (`/Game/VN_UI/BP_infolink_cutscene.MESSAGE` _returnvalue_6 "/Game/VN_UI/Avatars/T_Infolink_Hacker.T_Infolink_Hacker" "Ok, but watch your back. This island is not as deserted as your friend, the Wiz thought. People here are… special, so to speak. \nFortunately for you, they and I go way back, so you shouldn’t encounter any problems. Just be careful." "Hacker"))))

(event `Dialogue Lab terminal`
  (params (Line :type Integer :default 1))
  (switch `int` Line
    (:`0`
      (bind _returnvalue (`|CreateWidget` "/Game/VN_UI/BP_infolink_cutscene.BP_infolink_cutscene_C"))
      (`UserWidget.AddToViewport` _returnvalue 0)
      (`/Game/VN_UI/BP_infolink_cutscene.MESSAGE` _returnvalue "/Game/VN_UI/Avatars/T_Infolink_Hacker.T_Infolink_Hacker" " All right, find the terminal for the cell block’s door controls. Helsing should be inside." "Hacker"))
    (:`1`
      (bind _returnvalue_2 (`|CreateWidget` "/Game/VN_UI/BP_infolink_cutscene.BP_infolink_cutscene_C"))
      (`UserWidget.AddToViewport` _returnvalue_2 0)
      (`/Game/VN_UI/BP_infolink_cutscene.MESSAGE` _returnvalue_2 "/Game/VN_UI/Avatars/T_Infolink_Molly.T_Infolink_Molly" "Should? Why not \"is\"?" "Molly"))
    (:`2`
      (bind _returnvalue_3 (`|CreateWidget` "/Game/VN_UI/BP_infolink_cutscene.BP_infolink_cutscene_C"))
      (`UserWidget.AddToViewport` _returnvalue_3 0)
      (`/Game/VN_UI/BP_infolink_cutscene.MESSAGE` _returnvalue_3 "/Game/VN_UI/Avatars/T_Infolink_Hacker.T_Infolink_Hacker" "Well, signal scramblers fired up the moment you entered the lab. I hope R-Frames didn’t move him somewhere else. I could shut them down and gain control of the systems if you plug in me directly." "Hacker"))
    (:`3`
      (bind _returnvalue_4 (`|CreateWidget` "/Game/VN_UI/BP_infolink_cutscene.BP_infolink_cutscene_C"))
      (`UserWidget.AddToViewport` _returnvalue_4 0)
      (`/Game/VN_UI/BP_infolink_cutscene.MESSAGE` _returnvalue_4 "/Game/VN_UI/Avatars/T_Infolink_Hacker.T_Infolink_Hacker" "Our agreement stands: you help me, you help yourself. But hey, \nit’s a free country." "Hacker"))))

(event `Lab ending portal`
  (bind _returnvalue (`|CreateWidget` "/Game/VN_UI/BP_infolink_cutscene.BP_infolink_cutscene_C"))
  (`UserWidget.AddToViewport` _returnvalue 0)
  (`/Game/VN_UI/BP_infolink_cutscene.MESSAGE` _returnvalue "/Game/VN_UI/Avatars/T_Infolink_Hacker.T_Infolink_Hacker" "Get in the rift, quick!" "Hacker"))

(event `Ending 1`
  (params (Line :type Integer :default 1))
  (switch `int` Line
    (:`0`
      ;[1 1 1] ENDING 1
      (bind _returnvalue (`|CreateWidget` "/Game/VN_UI/BP_infolink_cutscene.BP_infolink_cutscene_C")) ; 0
      (`UserWidget.AddToViewport` _returnvalue 0)
      (`/Game/VN_UI/BP_infolink_cutscene.MESSAGE` _returnvalue "/Game/VN_UI/Avatars/T_Infolink_Hacker.T_Infolink_Hacker" "...so?" "Hacker"))
    (:`1`
      (bind _returnvalue_2 (`|CreateWidget` "/Game/VN_UI/BP_infolink_cutscene.BP_infolink_cutscene_C")) ; 1
      (`UserWidget.AddToViewport` _returnvalue_2 0)
      (`/Game/VN_UI/BP_infolink_cutscene.MESSAGE` _returnvalue_2 "/Game/VN_UI/Avatars/T_Infolink_Molly.T_Infolink_Molly" "It’s done." "Molly"))
    (:`2`
      (bind _returnvalue_3 (`|CreateWidget` "/Game/VN_UI/BP_infolink_cutscene.BP_infolink_cutscene_C")) ; 2
      (`UserWidget.AddToViewport` _returnvalue_3 0)
      (`/Game/VN_UI/BP_infolink_cutscene.MESSAGE` _returnvalue_3 "/Game/VN_UI/Avatars/T_Infolink_Molly.T_Infolink_Molly" "All in a day’s work, I guess." "Molly"))
    (:`3`
      (bind _returnvalue_4 (`|CreateWidget` "/Game/VN_UI/BP_infolink_cutscene.BP_infolink_cutscene_C")) ; 3
      (`UserWidget.AddToViewport` _returnvalue_4 0)
      (`/Game/VN_UI/BP_infolink_cutscene.MESSAGE` _returnvalue_4 "/Game/VN_UI/Avatars/T_Infolink_Hacker.T_Infolink_Hacker" "You’re free to go, Molly. Rest easy." "Hacker"))
    (:`4`
      (bind _returnvalue_5 (`|CreateWidget` "/Game/VN_UI/BP_infolink_cutscene.BP_infolink_cutscene_C")) ; 4
      (`UserWidget.AddToViewport` _returnvalue_5 0)
      (`/Game/VN_UI/BP_infolink_cutscene.MESSAGE` _returnvalue_5 "/Game/VN_UI/Avatars/T_Infolink_Hacker.T_Infolink_Hacker" "It’s time for someone else to pick up the pace, now." "Hacker"))
    (:`5`
      ;;[0.6518 1 0] NEWSCASTER
      (bind _returnvalue_6 (`|CreateWidget` "/Game/VN_UI/BP_infolink_cutscene.BP_infolink_cutscene_C")) ; 5
      (`UserWidget.AddToViewport` _returnvalue_6 0)
      (`/Game/VN_UI/BP_infolink_cutscene.MESSAGE` _returnvalue_6 "/Game/VN_UI/Avatars/noiser.noiser" "...and for the page about national news, the mysterious disappearance of Fortune 500 billionaire [INAUDIBLE]" "News reporter"))
    (:`6`
      (bind _returnvalue_7 (`|CreateWidget` "/Game/VN_UI/BP_infolink_cutscene.BP_infolink_cutscene_C")) ; 6
      (`UserWidget.AddToViewport` _returnvalue_7 0)
      (`/Game/VN_UI/BP_infolink_cutscene.MESSAGE` _returnvalue_7 "/Game/VN_UI/Avatars/noiser.noiser" "In 1996, a rapid explosion of underground fighting rings caused \nan unprecedented wave of arrests among the general populace. \n \nThe Galactamax Corporation, working with private prisons, drew from this growing stock of convicts, establishing a series of leagues and bloody public exhibitions." "News reporter"))
    (:`7`
      (bind _returnvalue_8 (`|CreateWidget` "/Game/VN_UI/BP_infolink_cutscene.BP_infolink_cutscene_C")) ; 7
      (`UserWidget.AddToViewport` _returnvalue_8 0)
      (`/Game/VN_UI/BP_infolink_cutscene.MESSAGE` _returnvalue_8 "/Game/VN_UI/Avatars/noiser.noiser" "The fight's popularity grew with their brutality. \nSoon, Galactamax discovered that the public matches were their most profitable enterprise. \n \nThe professional league was formed, the most vicious among these fighters being selected to fight in a Grand Tournament." "News reporter"))
    (:`8`
      (bind _returnvalue_9 (`|CreateWidget` "/Game/VN_UI/BP_infolink_cutscene.BP_infolink_cutscene_C")) ; 8
      (`UserWidget.AddToViewport` _returnvalue_9 0)
      (`/Game/VN_UI/BP_infolink_cutscene.MESSAGE` _returnvalue_9 "/Game/VN_UI/Avatars/noiser.noiser" "Many years have passed since the banning of Death Game. \nGalactamax has lost hundreds of millions in market value. \n \nWe don't know if the event of last night have any connection to Galactamax and their latest attempts at finding new venues for profit, but we'll do our best to keep you updated." "News reporter"))
    (:`9`
      (bind _returnvalue_10 (`|CreateWidget` "/Game/VN_UI/BP_infolink_cutscene.BP_infolink_cutscene_C")) ; 9
      (`UserWidget.AddToViewport` _returnvalue_10 0)
      (`/Game/VN_UI/BP_infolink_cutscene.MESSAGE` _returnvalue_10 "/Game/VN_UI/Avatars/noiser.noiser" "That would be all for now, thanks for watching. \n \nHave a great day." "News reporter"))
    (:`10`
      (bind _returnvalue_11 (`|CreateWidget` "/Game/VN_UI/BP_infolink_cutscene.BP_infolink_cutscene_C")) ; 10
      (`UserWidget.AddToViewport` _returnvalue_11 0)
      (`/Game/VN_UI/BP_infolink_cutscene.MESSAGE` _returnvalue_11 "/Game/VN_UI/Avatars/T_Infolink_Molly.T_Infolink_Molly" "We’re...free to go now, right?" "Molly"))
    (:`11`
      (bind _returnvalue_12 (`|CreateWidget` "/Game/VN_UI/BP_infolink_cutscene.BP_infolink_cutscene_C")) ; 11
      (`UserWidget.AddToViewport` _returnvalue_12 0)
      (`/Game/VN_UI/BP_infolink_cutscene.MESSAGE` _returnvalue_12 "/Game/VN_UI/Avatars/T_Infolink_Molly.T_Infolink_Molly" "I think I need to lie down." "Molly"))
    (:`12`
      ;;[0.5946 1 0] NEWSCASTER alt lines
      (bind _returnvalue_13 (`|CreateWidget` "/Game/VN_UI/BP_infolink_cutscene.BP_infolink_cutscene_C")) ; 12
      (`UserWidget.AddToViewport` _returnvalue_13 0)
      (`/Game/VN_UI/BP_infolink_cutscene.MESSAGE` _returnvalue_13 "/Game/VN_UI/Avatars/noiser.noiser" "As a figure equal parts influential and controversial, his disappearance comes as the shocking conclusion to the recent terror attacks on Galactamax by armed activist groups across the United States." "News reporter"))
    (:`13`
      (bind _returnvalue_14 (`|CreateWidget` "/Game/VN_UI/BP_infolink_cutscene.BP_infolink_cutscene_C")) ; 13
      (`UserWidget.AddToViewport` _returnvalue_14 0)
      (`/Game/VN_UI/BP_infolink_cutscene.MESSAGE` _returnvalue_14 "/Game/VN_UI/Avatars/noiser.noiser" "About 24 hours ago, federal agents managed to track down a group of individuals seemingly linked to the attack, which have since been taken into custody in a series of coordinated raids." "News reporter"))
    (:`14`
      (bind _returnvalue_15 (`|CreateWidget` "/Game/VN_UI/BP_infolink_cutscene.BP_infolink_cutscene_C")) ; 14
      (`UserWidget.AddToViewport` _returnvalue_15 0)
      (`/Game/VN_UI/BP_infolink_cutscene.MESSAGE` _returnvalue_15 "/Game/VN_UI/Avatars/noiser.noiser" "The Black-Hat terrorist known as “A.M.B.” was found to be part of this cell - and, after firing upon and critically injuring several agents , they were fatally wounded and successfully detained to a quarantined location." "News reporter"))
    (:`15`
      (bind _returnvalue_16 (`|CreateWidget` "/Game/VN_UI/BP_infolink_cutscene.BP_infolink_cutscene_C")) ; 15
      (`UserWidget.AddToViewport` _returnvalue_16 0)
      (`/Game/VN_UI/BP_infolink_cutscene.MESSAGE` _returnvalue_16 "/Game/VN_UI/Avatars/noiser.noiser" "The leader of the group, a Grey-Hat hacker claiming ties to the Department of Homeland Security, was detained without incident and is currently awaiting trial. It is speculated he may serve up to 300 years of imprisonment, along with total potential asset seizure in the event he may be unable to pay the damages inflicted to former Galactamax shareholders." "News reporter"))
    (:`16`
      (bind _returnvalue_17 (`|CreateWidget` "/Game/VN_UI/BP_infolink_cutscene.BP_infolink_cutscene_C")) ; 16
      (`UserWidget.AddToViewport` _returnvalue_17 0)
      (`/Game/VN_UI/BP_infolink_cutscene.MESSAGE` _returnvalue_17 "/Game/VN_UI/Avatars/noiser.noiser" "Federal authorities have already begun a nationwide search for the CEO, potentially coordinating with EuroPol as the case becomes further embroidered with political implications." "News reporter"))))

(fn `UserConstructionScript`)