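; Behavior tree task for the Episode 6 CEO mecha boss that performs a sumo move on the player within close range.
; It switches the player to a posed third-person camera, shakes it and plays a single-node animation on the mech.
; A FlipFlop alternates an Uwatenage throw, launching the player with health-scaled force, and a fast damaging Hatakikomi.
; It then restores first-person view and the animation Blueprint before finishing.
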(event `self.ReceiveExecuteAI`
  (params (OwnerController :type "AIController Object Reference") (ControlledPawn :type "Pawn Object Reference"))
  (bind _player (`/Game/Blueprints/NewFunctionLibrary.get player PURE`))
  (bind _player_2 (`/Game/Blueprints/NewFunctionLibrary.get player PURE`))
  (bind _asep6_ceomecha (cast `/Game/MISSIONS/EP6/Characters/EP6_CEOMECHA` ControlledPawn))
  (bind _returnvalue (`SceneComponent.K2_GetComponentLocation` (`Actor.RootComponent` _asep6_ceomecha)))
  (if (<= (`KismetMathLibrary.Vector_Distance` _returnvalue (`SceneComponent.K2_GetComponentLocation` (`Actor.RootComponent` _player_2))) 200.0) :!label _label
    (set `/Game/Blueprints/CHARACTERS/fpsMovementCharacter_light_1_vq3.cool 3p cam position` (`KismetMathLibrary.MakeVector` -90.0 -400.0 200.0) _player_2)
    (`/Game/Blueprints/CHARACTERS/fpsMovementCharacter_light_1_vq3.go 3p` _player_2 _returnvalue)
    (bind _mesh (`Character.Mesh` _asep6_ceomecha))
    (`SkeletalMeshComponent.SetAnimationMode` _mesh "AnimationSingleNode")
    (`PlayerCameraManager.PlayCameraShake` :`self` (`GameplayStatics.GetPlayerCameraManager` 0) :`ShakeClass` "/Game/Blueprints/SHAKES/BP_CameraShake_Hammer.BP_CameraShake_Hammer_C")
    (`/Engine/EditorBlueprintResources/StandardMacros.FlipFlop`
      (:`A`
        (`SkeletalMeshComponent.PlayAnimation` _mesh "/Game/MISSIONS/EP6/Characters/Uwatenage.Uwatenage" false)
        (`SkeletalMeshComponent.SetPlayRate` _mesh 0.5)
        (`KismetSystemLibrary.Delay` 0.3)
        (`Character.LaunchCharacter` _player (* (`KismetMathLibrary.GetForwardVector` (`Actor.K2_GetActorRotation` _asep6_ceomecha)) (* 15000.0 (/ (`/Game/Blueprints/CHARACTERS/fpsMovementCharacter_light_1_vq3.Health` _player) 100.0))) false false)
        (`KismetSystemLibrary.Delay` 0.7))
      (:`B`
        (`SkeletalMeshComponent.PlayAnimation` _mesh "/Game/MISSIONS/EP6/Characters/Hatakikomi.Hatakikomi" false)
        (`SkeletalMeshComponent.SetPlayRate` _mesh 5.0)
        (`GameplayStatics.ApplyDamage` _player 20.0)
        (`KismetSystemLibrary.Delay` 1.0)))
    (`/Game/Blueprints/CHARACTERS/fpsMovementCharacter_light_1_vq3.go 1p` _player_2)
    (`SkeletalMeshComponent.SetAnimationMode` (`Character.Mesh` _asep6_ceomecha) "AnimationBlueprint")
    (`|ExecutionSequence`
      (:`then_0`
        _)
      (:`then_1`
        (`KismetSystemLibrary.Delay` 1.0)
        (`/Engine/EditorBlueprintResources/StandardMacros.DoOnce` false :!pinned true :!via `Reset` ; Newcat just destroys everything with a punch.
          (:`Completed`
            (goto _label))))))
  (`self.FinishExecute` true))