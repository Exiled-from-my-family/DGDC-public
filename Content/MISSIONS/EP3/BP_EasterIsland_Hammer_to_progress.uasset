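; Floating skull obstacle for Easter Island that blocks a path and shoots at the player, meant to prompt a melee answer to a ranged threat.
; With clear sight, range and facing, it telegraphs a timeline charge, then fires twin railgun projectiles at the player's last seen position.
; Box overlap shows a "path closed" message.
; DISSOLVE! saves the SkullTag unlockable, fades and destroys the actor; BeginPlay removes it if already unlocked.
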(event `self.ReceiveTick`
  (params (DeltaSeconds :type "Float (single-precision)"))
  (bind _returnvalue (`GameplayStatics.GetPlayerPawn` 0))
  (bind _returnvalue_2 (`self.K2_GetActorLocation`))
  (bind _returnvalue_3 (`self.K2_GetActorLocation` _returnvalue))
  (bind _returnvalue_4 (`SceneComponent.K2_GetComponentLocation` (`self.Billboard`)))
  (bind _returnvalue_5 (`SceneComponent.K2_GetComponentLocation` (`self.Billboard1`)))
  ;[1 1 1] instead of being a wall, encourage the player to think about how to melee agaisnt a ranged threat.
  (bind (_outhit _returnvalue_6) (`KismetSystemLibrary.LineTraceSingle` _returnvalue_2 _returnvalue_3 "TraceTypeQuery1" false (`|MakeArray` _returnvalue :!type "Actor Object Reference")))
  (if _returnvalue_6
    (`|ExecutionSequence` :!label _label
      (:`then_0`
        (`Timeline|chargethen shoot` :!via `Stop` :!label _label_2
          (:`Finished`
            (`|SpawnActorFromClass` "/Game/Blueprints/PROJECTILES/BP_Proj_Railgun_Boss.BP_Proj_Railgun_Boss_C" (`KismetMathLibrary.MakeTransform` _returnvalue_4 (`KismetMathLibrary.FindLookAtRotation` _returnvalue_4 (stale _output_get))) "Undefined" "OverrideRootScale" null null)
            (`GameplayStatics.PlaySoundAtLocation` "/Game/AUDIO/SFX_Weapons/Weap_Robots/SC_Boss_shot.SC_Boss_shot" (stale _output_get) (struct) 1.0 1.0 0.0 null null null)
            (`|SpawnActorFromClass` "/Game/Blueprints/PROJECTILES/BP_Proj_Railgun_Boss.BP_Proj_Railgun_Boss_C" (`KismetMathLibrary.MakeTransform` _returnvalue_5 (`KismetMathLibrary.FindLookAtRotation` _returnvalue_5 (stale _output_get))) "Undefined" "OverrideRootScale" null null)
            (`PlayerCameraManager.PlayCameraShake` :`self` (`GameplayStatics.GetPlayerCameraManager` 0) :`ShakeClass` "/Game/Blueprints/SHAKES/BP_CameraShake_Jump_Heavy.BP_CameraShake_Jump_Heavy_C" :`Scale` 0.5)
            (`KismetSystemLibrary.Delay` 1.0)
            (if (`self.can shoot?`)
              (goto _label_3 :!via `Reset`)))))
      (:`then_1`
        (goto _label_3 :!via `Reset`)))
    (elif (and (> (.y (`KismetMathLibrary.InverseTransformLocation` (`self.GetTransform`) _returnvalue_3)) 0.0) (<= (`KismetMathLibrary.Vector_Distance` _returnvalue_2 _returnvalue_3) 2400.0))
      (`/Engine/EditorBlueprintResources/StandardMacros.DoOnce` false :!label _label_3
        (:`Completed`
          (`KismetSystemLibrary.Delay` 0.4)
          (bind _output_get (set `self.player last seen` _returnvalue_3))
          (if (`self.can shoot?`)
            (`GameplayStatics.SpawnEmitterAtLocation` "/Game/kosm_fps_assets/Misc/Particles/Blast/Effects/BlastParticles.BlastParticles" _output_get)
            (`GameplayStatics.PlaySoundAtLocation` "/Game/AUDIO/SFX_Damage/portalprojectile1.portalprojectile1" _returnvalue_3 (struct) 1.0 1.0 0.0 null null null)
            (bind _returnvalue_7 (`GameplayStatics.SpawnSoundAtLocation` "/Game/AUDIO/SC_Boss_ChargingUp.SC_Boss_ChargingUp" (`self.K2_GetActorLocation`) (struct) 1.0 1.0 0.0 null null))
            (set `self.charge SFX` _returnvalue_7)
            (`GameplayStatics.SpawnEmitterAttached` (`self.eyes VFX`) (`self.Billboard`) "None" (0.0 0.0 0.0) (struct) (0.5 0.5 0.5))
            (`GameplayStatics.SpawnEmitterAttached` (`self.eyes VFX`) (`self.Billboard1`) "None" (0.0 0.0 0.0) (struct) (0.5 0.5 0.5))
            (goto _label_2 :!via `PlayFromStart`))))
      (else
        (goto _label)))))

(event `DISSOLVE!`
  (bind _charge_sfx (`self.charge SFX`))
  ;[1 1 1] Magic! the object vanishes :DDD
  (`/Engine/EditorBlueprintResources/StandardMacros.DoOnce` false
    (:`Completed`
      (`/Game/Blueprints/NewFunctionLibrary.add unlockable` (`self.skull tag`))
      (`/Game/Blueprints/NewFunctionLibrary.clean all message widgets`)
      (set `self.can shoot?` false)
      (`self.SetActorEnableCollision` false)
      (`SceneComponent.SetVisibility` (`self.StaticMesh_Circle`) false false)
      (`LightComponent.SetIntensity` (`self.SpotLight`) 0.0)
      (`PrimitiveComponent.SetCollisionEnabled` (`self.Box`) "NoCollision")
      (`/Engine/EditorBlueprintResources/StandardMacros.IsValid` _charge_sfx
        (:`Is Valid`
          (`AudioComponent.Stop` _charge_sfx))
        (:`Is Not Valid`
          _))
      (`PlayerCameraManager.PlayCameraShake` :`self` (`GameplayStatics.GetPlayerCameraManager` 0) :`ShakeClass` "/Game/Blueprints/SHAKES/BP_CameraShake_Jump_Heavy.BP_CameraShake_Jump_Heavy_C" :`Scale` 2.0)
      (bind (_direction _newtrack_0) (`Timeline|Dissolve` :!via `PlayFromStart`)
        (:`Update`
          (`MeshComponent.SetScalarParameterValueOnMaterials` (`self.StaticMesh_A`) "Appearance" _newtrack_0)
          (`MeshComponent.SetScalarParameterValueOnMaterials` (`self.StaticMesh_B`) "Appearance" 0.0)
          (`MeshComponent.SetScalarParameterValueOnMaterials` (`self.StaticMesh_C`) "Appearance" 0.0)
          (goto _label_2 :!via `Stop`))
        (:`Finished`
          (`self.K2_DestroyActor`))))))

(event `self.ReceiveBeginPlay`
  (bind _unlocked_ (`/Game/Blueprints/NewFunctionLibrary.has unlockable` (`self.skull tag`)))
  (if _unlocked_
    (`self.K2_DestroyActor`)
    (else
      (`|ExecutionSequence`
        (:`then_0`
          (bind (_direction _newtrack_0) (`Timeline|Saturn ringz`)
            (:`Update`
              (bind _returnvalue (`KismetMathLibrary.Lerp` 0.0 359.0 _newtrack_0))
              (`SceneComponent.K2_SetRelativeRotation` (`self.StaticMesh_B`) (`KismetMathLibrary.MakeRotator` 0.0 (* _returnvalue -1.0)) false false)
              (`SceneComponent.K2_SetRelativeRotation` (`self.StaticMesh_C`) (`KismetMathLibrary.MakeRotator` 0.0 (/ _returnvalue 2.0)) false false))))
        (:`then_1`
          (bind (_direction_2 _floating) (`Timeline|Floating skull` :!via `PlayFromStart`)
            (:`Update`
              (`SceneComponent.K2_SetRelativeLocation` (`self.StaticMesh_A`) (`KismetMathLibrary.VLerp` (0.0 -132.5 5.0) (0.0 -132.5 -10.0) _floating) false false)
              (`SceneComponent.K2_SetRelativeLocation` (`self.StaticMesh_B`) (`KismetMathLibrary.VLerp` (0.0 -265.0 0.0) (0.0 -280.0 0.0) _floating) false false)
              (`SceneComponent.K2_SetRelativeLocation` (`self.StaticMesh_C`) (`KismetMathLibrary.VLerp` (0.0 -265.0 0.0) (0.0 -260.0 0.0) (/ _floating 0.5)) false false))))))))

(event `self.Box.OnComponentBeginOverlap`
  (params (OverlappedComponent :type "PrimitiveComponent Object Reference") (OtherActor :type "Actor Object Reference") (OtherComp :type "PrimitiveComponent Object Reference") (OtherBodyIndex :type Integer) (bFromSweep :type Boolean) (SweepResult :type "HitResult Structure (by ref)"))
  (cast `/Game/Blueprints/CHARACTERS/fpsMovementCharacter_light_1_vq3` OtherActor)
  (`/Engine/EditorBlueprintResources/StandardMacros.DoOnce` false :!label _label_4
    (:`Completed`
      (`/Game/Blueprints/NewFunctionLibrary.clean all message widgets`)
      (`KismetSystemLibrary.Delay` 0.01)
      (`GameplayStatics.PlaySound2D` "/Game/MISSIONS/EP2/Audio/SC_DoorLocked.SC_DoorLocked" 1.0 1.0 0.0 null null)
      (bind _returnvalue (`|CreateWidget` "/Game/Blueprints/UI/UI_Pickups/UI_GenericMessage.UI_GenericMessage_C"))
      (`UserWidget.AddToViewport` _returnvalue 0)
      (set `/Game/Blueprints/UI/UI_Pickups/UI_GenericMessage.Duration` 3.0 _returnvalue)
      (set `/Game/Blueprints/UI/UI_Pickups/UI_GenericMessage.Message` "This path is closed, for now..." _returnvalue)
      (`KismetSystemLibrary.Delay` 0.2)
      (goto _label_4 :!via `Reset`))))

(fn `UserConstructionScript`
  (bind _staticmesh_a (`self.StaticMesh_A`))
  (bind _staticmesh_b (`self.StaticMesh_B`))
  (bind _staticmesh_c (`self.StaticMesh_C`))
  (`PrimitiveComponent.CreateDynamicMaterialInstance` _staticmesh_a 0 "/Game/Blueprints/MISC/M_HammerObstacle_Inst.M_HammerObstacle_Inst" "None")
  (`MeshComponent.SetScalarParameterValueOnMaterials` _staticmesh_a "Appearance" 1.0)
  (`PrimitiveComponent.CreateDynamicMaterialInstance` _staticmesh_b 0 "/Game/Blueprints/MISC/M_HammerObstacle_Inst1.M_HammerObstacle_Inst1" "None")
  (`MeshComponent.SetScalarParameterValueOnMaterials` _staticmesh_b "Appearance" 1.0)
  (`PrimitiveComponent.CreateDynamicMaterialInstance` _staticmesh_c 0 "/Game/Blueprints/MISC/M_HammerObstacle_Inst1.M_HammerObstacle_Inst1" "None")
  (`MeshComponent.SetScalarParameterValueOnMaterials` _staticmesh_c "Appearance" 1.0))