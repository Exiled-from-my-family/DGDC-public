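; Cinematic dialogue Blueprint for Episode 3 that supplies the infolink lines for CTF, lobby, island and lab cutscenes, plus an episode-end exchange.
; Each scene has a custom event that takes a line index and creates a BP_infolink_cutscene widget with avatar, text and speaker, including alternate lines for story branches.
; Lines are skippable except the episode-end exchange.
; Helper events restore the HUD and clear those widgets, play hacker music, or call SpawnLG.
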(event `SPAWN LG`
  (`self.SpawnLG`))

(event `CTF1_Hackmusic`
  (`GameplayStatics.SpawnSound2D` "/Game/MISSIONS/EP3/Music/SC_CTF1_Hacker.SC_CTF1_Hacker" 0.7 1.0 0.0 null))

(event `Quit`
  (bind _player (`/Game/Blueprints/NewFunctionLibrary.get player`))
  (`Widget.SetVisibility` (`/Game/Blueprints/CHARACTERS/fpsMovementCharacter_light_1_vq3.HUD` _player) "Visible")
  (bind _foundwidgets (`WidgetBlueprintLibrary.GetAllWidgetsOfClass` "/Game/VN_UI/BP_infolink_cutscene.BP_infolink_cutscene_C"))
  (`Widget.RemoveFromParent` _foundwidgets))

(event `Dialogue Lab helsing`
  (params (Line :type Integer :default 1))
  (switch `int` Line
    (:`0`
      (bind _returnvalue (`|CreateWidget` "/Game/VN_UI/BP_infolink_cutscene.BP_infolink_cutscene_C"))
      (`UserWidget.AddToViewport` _returnvalue 0)
      (`/Game/VN_UI/BP_infolink_cutscene.MESSAGE` _returnvalue "/Game/VN_UI/Avatars/T_Infolink_Molly.T_Infolink_Molly" "Ok. We’re fucked. I’m fucked!" "Molly"))
    (:`1`
      (bind _returnvalue_2 (`|CreateWidget` "/Game/VN_UI/BP_infolink_cutscene.BP_infolink_cutscene_C"))
      (`UserWidget.AddToViewport` _returnvalue_2 0)
      (`/Game/VN_UI/BP_infolink_cutscene.MESSAGE` _returnvalue_2 "/Game/VN_UI/Avatars/T_Infolink_Hacker.T_Infolink_Hacker" "He’s not there? I suspected as much." "Hacker"))
    (:`2`
      (bind _returnvalue_3 (`|CreateWidget` "/Game/VN_UI/BP_infolink_cutscene.BP_infolink_cutscene_C"))
      (`UserWidget.AddToViewport` _returnvalue_3 0)
      (`/Game/VN_UI/BP_infolink_cutscene.MESSAGE` _returnvalue_3 "/Game/VN_UI/Avatars/T_Infolink_Molly.T_Infolink_Molly" "Well, why didn’t you tell me? The hell am I going to do now? I’m at the bottom of a black site in the tropics, I can’t just pop out to the beach like nothing happened!" "Molly"))
    (:`3`
      (bind _returnvalue_4 (`|CreateWidget` "/Game/VN_UI/BP_infolink_cutscene.BP_infolink_cutscene_C"))
      (`UserWidget.AddToViewport` _returnvalue_4 0)
      (`/Game/VN_UI/BP_infolink_cutscene.MESSAGE` _returnvalue_4 "/Game/VN_UI/Avatars/T_Infolink_Hacker.T_Infolink_Hacker" "That might be the best thing to do right now. We have time for a quick exfil. \nUnfortunately I tripped a silent alarm. You have tangos incoming. \nBUT! I did find something interesting in one of the armories." "Hacker"))
    (:`4`
      (bind _returnvalue_5 (`|CreateWidget` "/Game/VN_UI/BP_infolink_cutscene.BP_infolink_cutscene_C"))
      (`UserWidget.AddToViewport` _returnvalue_5 0)
      (`/Game/VN_UI/BP_infolink_cutscene.MESSAGE` _returnvalue_5 "/Game/VN_UI/Avatars/T_Infolink_Hacker.T_Infolink_Hacker" "Going dark now, see you topside." "Hacker"))
    (:`5`
      (bind _returnvalue_6 (`|CreateWidget` "/Game/VN_UI/BP_infolink_cutscene.BP_infolink_cutscene_C"))
      (`UserWidget.AddToViewport` _returnvalue_6 0)
      (`/Game/VN_UI/BP_infolink_cutscene.MESSAGE` _returnvalue_6 "/Game/VN_UI/Avatars/T_Infolink_Hacker.T_Infolink_Hacker" "That might be the best thing to do right now. We have time for a quick exfil. \nUnfortunately I tripped a silent alarm. You have tangos incoming. \nTry to stay to alive. Going dark now, good luck." "Hacker"))))

(event `EPISODE 1 END`
  (params (Line :type Integer :default 1))
  (switch `int` Line
    (:`0`
      (bind _returnvalue (`|CreateWidget` "/Game/VN_UI/BP_infolink_cutscene.BP_infolink_cutscene_C" null false))
      (`UserWidget.AddToViewport` _returnvalue 0)
      (`/Game/VN_UI/BP_infolink_cutscene.MESSAGE` _returnvalue "/Game/Blueprints/DISSOLVE_VFX/Textures/Mobile/T_Noise_7_256.T_Noise_7_256" "Hello?" " "))
    (:`1`
      (bind _returnvalue_2 (`|CreateWidget` "/Game/VN_UI/BP_infolink_cutscene.BP_infolink_cutscene_C" null false))
      (`UserWidget.AddToViewport` _returnvalue_2 0)
      (`/Game/VN_UI/BP_infolink_cutscene.MESSAGE` _returnvalue_2 "/Game/Blueprints/DISSOLVE_VFX/Textures/Standart/T_Noise_8.T_Noise_8" " ...Sir? Did you receive the footage?" ""))
    (:`2`
      (bind _returnvalue_3 (`|CreateWidget` "/Game/VN_UI/BP_infolink_cutscene.BP_infolink_cutscene_C" null false))
      (`UserWidget.AddToViewport` _returnvalue_3 0)
      (`/Game/VN_UI/BP_infolink_cutscene.MESSAGE` _returnvalue_3 "/Game/Blueprints/DISSOLVE_VFX/Textures/Mobile/T_Noise_7_256.T_Noise_7_256" "Yes, I did. A sight to behold." " "))
    (:`3`
      (bind _returnvalue_4 (`|CreateWidget` "/Game/VN_UI/BP_infolink_cutscene.BP_infolink_cutscene_C" null false))
      (`UserWidget.AddToViewport` _returnvalue_4 0)
      (`/Game/VN_UI/BP_infolink_cutscene.MESSAGE` _returnvalue_4 "/Game/Blueprints/DISSOLVE_VFX/Textures/Standart/T_Noise_8.T_Noise_8" "How should we proceed? I’m at a loss." ""))
    (:`4`
      (bind _returnvalue_5 (`|CreateWidget` "/Game/VN_UI/BP_infolink_cutscene.BP_infolink_cutscene_C" null false))
      (`UserWidget.AddToViewport` _returnvalue_5 0)
      (`/Game/VN_UI/BP_infolink_cutscene.MESSAGE` _returnvalue_5 "/Game/Blueprints/DISSOLVE_VFX/Textures/Mobile/T_Noise_7_256.T_Noise_7_256" "That’s two of us then. But for different reasons." " "))
    (:`5`
      (bind _returnvalue_6 (`|CreateWidget` "/Game/VN_UI/BP_infolink_cutscene.BP_infolink_cutscene_C" null false))
      (`UserWidget.AddToViewport` _returnvalue_6 0)
      (`/Game/VN_UI/BP_infolink_cutscene.MESSAGE` _returnvalue_6 "/Game/Blueprints/DISSOLVE_VFX/Textures/Mobile/T_Noise_7_256.T_Noise_7_256" "This is going to be a long day." " "))))

(event `Dialogue Island Gmax discovery`
  (params (Line :type Integer :default 1))
  ;[1 1 1] CTF3 Gmax discovery
  (switch `int` Line
    (:`0`
      (bind _returnvalue (`|CreateWidget` "/Game/VN_UI/BP_infolink_cutscene.BP_infolink_cutscene_C")) ; 0
      (`UserWidget.AddToViewport` _returnvalue 0)
      (`/Game/VN_UI/BP_infolink_cutscene.MESSAGE` _returnvalue "/Game/VN_UI/Avatars/T_Infolink_Hacker.T_Infolink_Hacker" "Hold it, don’t go any further!" "Hacker"))
    (:`1`
      (bind _returnvalue_2 (`|CreateWidget` "/Game/VN_UI/BP_infolink_cutscene.BP_infolink_cutscene_C"))
      (`UserWidget.AddToViewport` _returnvalue_2 0)
      (`/Game/VN_UI/BP_infolink_cutscene.MESSAGE` _returnvalue_2 "/Game/VN_UI/Avatars/T_Infolink_Molly.T_Infolink_Molly" "Did not plan to. This place looks like trouble." "Molly"))
    (:`2`
      (bind _returnvalue_3 (`|CreateWidget` "/Game/VN_UI/BP_infolink_cutscene.BP_infolink_cutscene_C"))
      (`UserWidget.AddToViewport` _returnvalue_3 0)
      (`/Game/VN_UI/BP_infolink_cutscene.MESSAGE` _returnvalue_3 "/Game/VN_UI/Avatars/T_Infolink_Hacker.T_Infolink_Hacker" "Yes, this is a covert Galactamax facility." "Hacker"))
    (:`3`
      (bind _returnvalue_4 (`|CreateWidget` "/Game/VN_UI/BP_infolink_cutscene.BP_infolink_cutscene_C"))
      (`UserWidget.AddToViewport` _returnvalue_4 0)
      (`/Game/VN_UI/BP_infolink_cutscene.MESSAGE` _returnvalue_4 "/Game/VN_UI/Avatars/T_Infolink_Molly.T_Infolink_Molly" "What? Like, the billion-dollar corp? The one that started blood sports entertainment?" "Molly"))
    (:`4`
      (bind _returnvalue_5 (`|CreateWidget` "/Game/VN_UI/BP_infolink_cutscene.BP_infolink_cutscene_C"))
      (`UserWidget.AddToViewport` _returnvalue_5 0)
      (`/Game/VN_UI/BP_infolink_cutscene.MESSAGE` _returnvalue_5 "/Game/VN_UI/Avatars/T_Infolink_Hacker.T_Infolink_Hacker" "Yeah, but the name was different back then. And they had a show…" "Hacker"))
    (:`5`
      (bind _returnvalue_6 (`|CreateWidget` "/Game/VN_UI/BP_infolink_cutscene.BP_infolink_cutscene_C"))
      (`UserWidget.AddToViewport` _returnvalue_6 0)
      (`/Game/VN_UI/BP_infolink_cutscene.MESSAGE` _returnvalue_6 "/Game/VN_UI/Avatars/T_Infolink_Molly.T_Infolink_Molly" "I remember! \"Death Game”. I think one of my cousins was a fan – convicts shooting each other with stupidly big guns.  \nCan’t believe this was on the TV. It ran for a few years, right? And then it got banned." "Molly"))
    (:`6`
      (bind _returnvalue_7 (`|CreateWidget` "/Game/VN_UI/BP_infolink_cutscene.BP_infolink_cutscene_C"))
      (`UserWidget.AddToViewport` _returnvalue_7 0)
      (`/Game/VN_UI/BP_infolink_cutscene.MESSAGE` _returnvalue_7 "/Game/VN_UI/Avatars/T_Infolink_Hacker.T_Infolink_Hacker" "Bingo. It was outlawed with the Lieb/Kohn Act. The company stayed afloat though – and became Galactamax. And they could afford black sites, like this one. \nI don’t think we can handle that, there are a lot of heat signatures there, including non-human. Let’s go get that flag instead." "Hacker"))))

(event `Dialogue island part 2_1`
  (params (Line :type Integer :default 1))
  ;[1 1 1] CTF3 Part 2 -1
  (switch `int` Line
    (:`0`
      (bind _returnvalue (`|CreateWidget` "/Game/VN_UI/BP_infolink_cutscene.BP_infolink_cutscene_C")) ; 0
      (`UserWidget.AddToViewport` _returnvalue 0)
      (`/Game/VN_UI/BP_infolink_cutscene.MESSAGE` _returnvalue "/Game/VN_UI/Avatars/T_Infolink_Hacker.T_Infolink_Hacker" "Shit, they’re here. Stay low." "Hacker"))
    (:`1`
      (bind _returnvalue_2 (`|CreateWidget` "/Game/VN_UI/BP_infolink_cutscene.BP_infolink_cutscene_C"))
      (`UserWidget.AddToViewport` _returnvalue_2 0)
      (`/Game/VN_UI/BP_infolink_cutscene.MESSAGE` _returnvalue_2 "/Game/VN_UI/Avatars/Arcade_avatars/T_Arc_Rframe.T_Arc_Rframe" "Control, Spear 48: Perimeter breach. Executing full response." "R-Frame"))
    (:`2`
      (bind _returnvalue_3 (`|CreateWidget` "/Game/VN_UI/BP_infolink_cutscene.BP_infolink_cutscene_C"))
      (`UserWidget.AddToViewport` _returnvalue_3 0)
      (`/Game/VN_UI/BP_infolink_cutscene.MESSAGE` _returnvalue_3 "/Game/VN_UI/Avatars/T_Infolink_MajorCommando.T_Infolink_MajorCommando" "Woah, we’re just standing here!" "Major"))
    (:`3`
      (bind _returnvalue_4 (`|CreateWidget` "/Game/VN_UI/BP_infolink_cutscene.BP_infolink_cutscene_C"))
      (`UserWidget.AddToViewport` _returnvalue_4 0)
      (`/Game/VN_UI/BP_infolink_cutscene.MESSAGE` _returnvalue_4 "/Game/VN_UI/Avatars/T_Infolink_Wizard.T_Infolink_Wizard" "Enough! I’m getting us outta here!" "Wizard"))
    (:`4`
      (bind _returnvalue_5 (`|CreateWidget` "/Game/VN_UI/BP_infolink_cutscene.BP_infolink_cutscene_C"))
      (`UserWidget.AddToViewport` _returnvalue_5 0)
      (`/Game/VN_UI/BP_infolink_cutscene.MESSAGE` _returnvalue_5 "/Game/VN_UI/Avatars/T_Infolink_Rumbletron.T_Infolink_Rumbletron" "Wait! What about [Molly, Molly, Mo-] and the [Vampire Savior]?" "Rumbletron"))
    (:`5`
      (bind _returnvalue_6 (`|CreateWidget` "/Game/VN_UI/BP_infolink_cutscene.BP_infolink_cutscene_C"))
      (`UserWidget.AddToViewport` _returnvalue_6 0)
      (`/Game/VN_UI/BP_infolink_cutscene.MESSAGE` _returnvalue_6 "/Game/VN_UI/Avatars/Arcade_avatars/T_Arc_Rframe.T_Arc_Rframe" "Target lost. Sweep and resume." "R-Frame"))
    (:`6`
      (bind _returnvalue_7 (`|CreateWidget` "/Game/VN_UI/BP_infolink_cutscene.BP_infolink_cutscene_C"))
      (`UserWidget.AddToViewport` _returnvalue_7 0)
      (`/Game/VN_UI/BP_infolink_cutscene.MESSAGE` _returnvalue_7 "/Game/VN_UI/Avatars/T_Infolink_Hacker.T_Infolink_Hacker" "Hide, quick! And don’t move!" "Hacker"))))

(event `Dialogue Island stranded`
  (params (Line :type Integer :default 1))
  ;[1 1 1] CTF3 stranded
  (switch `int` Line
    (:`0`
      (bind _returnvalue (`|CreateWidget` "/Game/VN_UI/BP_infolink_cutscene.BP_infolink_cutscene_C")) ; 0
      (`UserWidget.AddToViewport` _returnvalue 0)
      (`/Game/VN_UI/BP_infolink_cutscene.MESSAGE` _returnvalue "/Game/VN_UI/Avatars/T_Infolink_Molly.T_Infolink_Molly" "Ok, what now?" "Molly"))
    (:`1`
      (bind _returnvalue_2 (`|CreateWidget` "/Game/VN_UI/BP_infolink_cutscene.BP_infolink_cutscene_C")) ; 1 - hack w/o r frames
      (`UserWidget.AddToViewport` _returnvalue_2 0)
      (`/Game/VN_UI/BP_infolink_cutscene.MESSAGE` _returnvalue_2 "/Game/VN_UI/Avatars/T_Infolink_Hacker.T_Infolink_Hacker" "This is bad. Now, I’ve been sweeping the base you found and discovered a negative thermal signature in one of the holding cells." "Hacker"))
    (:`2`
      (bind _returnvalue_3 (`|CreateWidget` "/Game/VN_UI/BP_infolink_cutscene.BP_infolink_cutscene_C")) ; 2 - hack w/ r frame
      (`UserWidget.AddToViewport` _returnvalue_3 0)
      (`/Game/VN_UI/BP_infolink_cutscene.MESSAGE` _returnvalue_3 "/Game/VN_UI/Avatars/T_Infolink_Hacker.T_Infolink_Hacker" "This is bad. Now, I’ve been checking on movements of R-Frames, as well as sweeping the base you found and discovered negative thermal signature in one of the holding cells." "Hacker"))
    (:`3`
      (bind _returnvalue_4 (`|CreateWidget` "/Game/VN_UI/BP_infolink_cutscene.BP_infolink_cutscene_C")) ; 3  - molly w/o r frame
      (`UserWidget.AddToViewport` _returnvalue_4 0)
      (`/Game/VN_UI/BP_infolink_cutscene.MESSAGE` _returnvalue_4 "/Game/VN_UI/Avatars/T_Infolink_Molly.T_Infolink_Molly" "So, that's Helsing, probably, right?" "Molly"))
    (:`4`
      (bind _returnvalue_5 (`|CreateWidget` "/Game/VN_UI/BP_infolink_cutscene.BP_infolink_cutscene_C")) ; 4 - molly w/ r frame
      (`UserWidget.AddToViewport` _returnvalue_5 0)
      (`/Game/VN_UI/BP_infolink_cutscene.MESSAGE` _returnvalue_5 "/Game/VN_UI/Avatars/T_Infolink_Molly.T_Infolink_Molly" "So, that's Helsing, probably, right?  And what the hell is an R-Frame?" "Molly"))
    (:`5`
      (bind _returnvalue_6 (`|CreateWidget` "/Game/VN_UI/BP_infolink_cutscene.BP_infolink_cutscene_C")) ; 5 - hack w/o r frame
      (`UserWidget.AddToViewport` _returnvalue_6 0)
      (`/Game/VN_UI/BP_infolink_cutscene.MESSAGE` _returnvalue_6 "/Game/VN_UI/Avatars/T_Infolink_Hacker.T_Infolink_Hacker" "Yes. Now, I managed to initiate the evacuation protocol. The whole place, apart from sentries, is deserted for now. It’s our chance – yours for saving Helsing, mine for getting a better picture of what they’re planning here." "Hacker"))
    (:`6`
      (bind _returnvalue_7 (`|CreateWidget` "/Game/VN_UI/BP_infolink_cutscene.BP_infolink_cutscene_C")) ; 6 - hack w r frame
      (`UserWidget.AddToViewport` _returnvalue_7 0)
      (`/Game/VN_UI/BP_infolink_cutscene.MESSAGE` _returnvalue_7 "/Game/VN_UI/Avatars/T_Infolink_Hacker.T_Infolink_Hacker" "Those robots are called R-Frames. Supposedly in the experimental stage. Built by Galactamax. The Wiz must have stumbled into a testing ground." "Hacker"))
    (:`7`
      (bind _returnvalue_8 (`|CreateWidget` "/Game/VN_UI/BP_infolink_cutscene.BP_infolink_cutscene_C")) ; 7 - molly  gmax
      (`UserWidget.AddToViewport` _returnvalue_8 0)
      (`/Game/VN_UI/BP_infolink_cutscene.MESSAGE` _returnvalue_8 "/Game/VN_UI/Avatars/T_Infolink_Molly.T_Infolink_Molly" "What? Like, the billion-dollar corp? The one that started blood sports entertainment?" "Molly"))
    (:`8`
      (bind _returnvalue_9 (`|CreateWidget` "/Game/VN_UI/BP_infolink_cutscene.BP_infolink_cutscene_C")) ; 8 - hack gmax_1
      (`UserWidget.AddToViewport` _returnvalue_9 0)
      (`/Game/VN_UI/BP_infolink_cutscene.MESSAGE` _returnvalue_9 "/Game/VN_UI/Avatars/T_Infolink_Hacker.T_Infolink_Hacker" "Yeah, but the name was different back then. And they had a show…" "Hacker"))
    (:`9`
      (bind _returnvalue_10 (`|CreateWidget` "/Game/VN_UI/BP_infolink_cutscene.BP_infolink_cutscene_C")) ; 9 - molly  gmax
      (`UserWidget.AddToViewport` _returnvalue_10 0)
      (`/Game/VN_UI/BP_infolink_cutscene.MESSAGE` _returnvalue_10 "/Game/VN_UI/Avatars/T_Infolink_Molly.T_Infolink_Molly" "I remember! \"Death Game”. I think one of my cousins was a fan – convicts shooting each other with stupidly big guns. Can’t believe this was on the TV. It ran for a few years, right? And then it got banned." "Molly"))
    (:`10`
      (bind _returnvalue_11 (`|CreateWidget` "/Game/VN_UI/BP_infolink_cutscene.BP_infolink_cutscene_C")) ; 10 - hack gmax_2
      (`UserWidget.AddToViewport` _returnvalue_11 0)
      (`/Game/VN_UI/BP_infolink_cutscene.MESSAGE` _returnvalue_11 "/Game/VN_UI/Avatars/T_Infolink_Hacker.T_Infolink_Hacker" "Bingo. It was outlawed with the Lieb/Kohn Act. The company stayed afloat though – and became Galactamax. And they could afford black sites, like this one." "Hacker"))
    (:`11`
      (bind _returnvalue_12 (`|CreateWidget` "/Game/VN_UI/BP_infolink_cutscene.BP_infolink_cutscene_C")) ; 11 - hack w/o r frame
      (`UserWidget.AddToViewport` _returnvalue_12 0)
      (`/Game/VN_UI/BP_infolink_cutscene.MESSAGE` _returnvalue_12 "/Game/VN_UI/Avatars/T_Infolink_Hacker.T_Infolink_Hacker" "Now, I managed to initiate the evacuation protocol. The whole place, apart from sentries, is deserted for now. It’s our chance – yours for saving Helsing, mine for getting a better picture of what they’re planning here." "Hacker"))))

(event `Dialogues Island intro`
  (params (Line :type Integer :default 1))
  (switch `int` Line
    (:`0`
      ;[1 1 1] CTF3 intro
      (bind _returnvalue (`|CreateWidget` "/Game/VN_UI/BP_infolink_cutscene.BP_infolink_cutscene_C")) ; 0
      (`UserWidget.AddToViewport` _returnvalue 0)
      (`/Game/VN_UI/BP_infolink_cutscene.MESSAGE` _returnvalue "/Game/VN_UI/Avatars/T_Infolink_Wizard.T_Infolink_Wizard" "Ok, you’re all here, superb. This map is special. It is the variant of CTF thought to be quite controversial in the old days – One Flag.  \nSo… one team attacks, the other – defends." "Wizard"))
    (:`1`
      (bind _returnvalue_2 (`|CreateWidget` "/Game/VN_UI/BP_infolink_cutscene.BP_infolink_cutscene_C"))
      (`UserWidget.AddToViewport` _returnvalue_2 0)
      (`/Game/VN_UI/BP_infolink_cutscene.MESSAGE` _returnvalue_2 "/Game/VN_UI/Avatars/T_Infolink_Molly.T_Infolink_Molly" "Wait… Is it me or my whole body is heavier now? I had some trouble breathing and now… I feel slow. Did you do something with the gravity?" "Molly"))
    (:`2`
      (bind _returnvalue_3 (`|CreateWidget` "/Game/VN_UI/BP_infolink_cutscene.BP_infolink_cutscene_C"))
      (`UserWidget.AddToViewport` _returnvalue_3 0)
      (`/Game/VN_UI/BP_infolink_cutscene.MESSAGE` _returnvalue_3 "/Game/VN_UI/Avatars/T_Infolink_MajorCommando.T_Infolink_MajorCommando" "Yeah, I feel dizzy as well. Haven’t felt this way since my days of hitting dope in Da Nang." "Major"))
    (:`3`
      (bind _returnvalue_4 (`|CreateWidget` "/Game/VN_UI/BP_infolink_cutscene.BP_infolink_cutscene_C"))
      (`UserWidget.AddToViewport` _returnvalue_4 0)
      (`/Game/VN_UI/BP_infolink_cutscene.MESSAGE` _returnvalue_4 "/Game/VN_UI/Avatars/T_Infolink_Wizard.T_Infolink_Wizard" "Things are under control. It’s just… Well… We MIGHT be on a real tropical island in the real world now." "Wizard"))
    (:`4`
      (bind _returnvalue_5 (`|CreateWidget` "/Game/VN_UI/BP_infolink_cutscene.BP_infolink_cutscene_C"))
      (`UserWidget.AddToViewport` _returnvalue_5 0)
      (`/Game/VN_UI/BP_infolink_cutscene.MESSAGE` _returnvalue_5 "/Game/VN_UI/Avatars/T_Infolink_FlakJack.T_Infolink_FlakJack" "Sweet Mother Mary..." "Flak Jack"))
    (:`5`
      (bind _returnvalue_6 (`|CreateWidget` "/Game/VN_UI/BP_infolink_cutscene.BP_infolink_cutscene_C"))
      (`UserWidget.AddToViewport` _returnvalue_6 0)
      (`/Game/VN_UI/BP_infolink_cutscene.MESSAGE` _returnvalue_6 "/Game/VN_UI/Avatars/T_Infolink_Molly.T_Infolink_Molly" "So we are haunting the place now? Like a bunch of poltergeists? How that fuck is that even possible?!" "Molly"))
    (:`6`
      (bind _returnvalue_7 (`|CreateWidget` "/Game/VN_UI/BP_infolink_cutscene.BP_infolink_cutscene_C"))
      (`UserWidget.AddToViewport` _returnvalue_7 0)
      (`/Game/VN_UI/BP_infolink_cutscene.MESSAGE` _returnvalue_7 "/Game/VN_UI/Avatars/T_Infolink_Wizard.T_Infolink_Wizard" "Stop. We are not in the real world yet. Not completely.  \nThis is a Dimensional Rupture Zone. We’re halfway one dimension – mine – and the real world. Some parts of my arena should be scattered on the island. Such as the blue flag, which probably is in a nearby temple." "Wizard"))
    (:`7`
      (bind _returnvalue_8 (`|CreateWidget` "/Game/VN_UI/BP_infolink_cutscene.BP_infolink_cutscene_C"))
      (`UserWidget.AddToViewport` _returnvalue_8 0)
      (`/Game/VN_UI/BP_infolink_cutscene.MESSAGE` _returnvalue_8 "/Game/VN_UI/Avatars/T_Infolink_Wendy.T_Infolink_Wendy" "Wait… And what if WE get shot? Does this zone use game world’s rules or…?" "Wendy"))
    (:`8`
      (bind _returnvalue_9 (`|CreateWidget` "/Game/VN_UI/BP_infolink_cutscene.BP_infolink_cutscene_C"))
      (`UserWidget.AddToViewport` _returnvalue_9 0)
      (`/Game/VN_UI/BP_infolink_cutscene.MESSAGE` _returnvalue_9 "/Game/VN_UI/Avatars/T_Infolink_Wizard.T_Infolink_Wizard" "Well, you should be revived. Unfortunately the implications of combat in Rupture Zone escape me. Mostly because no-one ever fought in one. Also, wait…where is Helsing?" "Wizard"))
    (:`9`
      (bind _returnvalue_10 (`|CreateWidget` "/Game/VN_UI/BP_infolink_cutscene.BP_infolink_cutscene_C"))
      (`UserWidget.AddToViewport` _returnvalue_10 0)
      (`/Game/VN_UI/BP_infolink_cutscene.MESSAGE` _returnvalue_10 "/Game/VN_UI/Avatars/T_Infolink_Wizard.T_Infolink_Wizard" "Ok, someone go grab the flag and find him, while I think about sewing the rupture back together." "Wizard"))
    (:`10`
      (bind _returnvalue_11 (`|CreateWidget` "/Game/VN_UI/BP_infolink_cutscene.BP_infolink_cutscene_C"))
      (`UserWidget.AddToViewport` _returnvalue_11 0)
      (`/Game/VN_UI/BP_infolink_cutscene.MESSAGE` _returnvalue_11 "/Game/VN_UI/Avatars/T_Infolink_FlakJack.T_Infolink_FlakJack" "Ugh, the five hundred pounds of armor on my back really started to weigh on me. Tell you what. I’m gonna set up camp, you lot think about that flag." "Flak Jack"))
    (:`11`
      (bind _returnvalue_12 (`|CreateWidget` "/Game/VN_UI/BP_infolink_cutscene.BP_infolink_cutscene_C"))
      (`UserWidget.AddToViewport` _returnvalue_12 0)
      (`/Game/VN_UI/BP_infolink_cutscene.MESSAGE` _returnvalue_12 "/Game/VN_UI/Avatars/T_Infolink_Molly.T_Infolink_Molly" "Well, I’m tired of asking questions, I’ll just go..." "Molly"))
    (:`12`
      (bind _returnvalue_13 (`|CreateWidget` "/Game/VN_UI/BP_infolink_cutscene.BP_infolink_cutscene_C"))
      (`UserWidget.AddToViewport` _returnvalue_13 0)
      (`/Game/VN_UI/BP_infolink_cutscene.MESSAGE` _returnvalue_13 "/Game/VN_UI/Avatars/T_Infolink_Rumbletron.T_Infolink_Rumbletron" "This island… [I’VE JUST BEEN IN THIS PLACE BEFORE!] Something bad happened here." "Rumbletron"))))

(event `Dialogue cutscenes`
  (params (Line :type Integer :default 1))
  (switch `int` Line
    (:`0`
      ;[1 1 1] CTF BLACKOUT
      (bind _returnvalue (`|CreateWidget` "/Game/VN_UI/BP_infolink_cutscene.BP_infolink_cutscene_C")) ; 0
      (`UserWidget.AddToViewport` _returnvalue 0)
      (`/Game/VN_UI/BP_infolink_cutscene.MESSAGE` _returnvalue "/Game/VN_UI/Avatars/T_Infolink_Hacker.T_Infolink_Hacker" "I’m in." "Hacker"))
    (:`1`
      (bind _returnvalue_2 (`|CreateWidget` "/Game/VN_UI/BP_infolink_cutscene.BP_infolink_cutscene_C"))
      (`UserWidget.AddToViewport` _returnvalue_2 0)
      (`/Game/VN_UI/BP_infolink_cutscene.MESSAGE` _returnvalue_2 "/Game/VN_UI/Avatars/T_Infolink_Molly.T_Infolink_Molly" "Oh, you… you’re that…ummm..." "Molly"))
    (:`2`
      (bind _returnvalue_3 (`|CreateWidget` "/Game/VN_UI/BP_infolink_cutscene.BP_infolink_cutscene_C"))
      (`UserWidget.AddToViewport` _returnvalue_3 0)
      (`/Game/VN_UI/BP_infolink_cutscene.MESSAGE` _returnvalue_3 "/Game/VN_UI/Avatars/T_Infolink_Hacker.T_Infolink_Hacker" "A specialist. I work for the government as, let’s just say, intelligence officer.  \nYour \"friend\", the Wizard? What he’s dabbling in goes far beyond this necromantic freakshow. \nSo, do you want to leave?" "Hacker"))
    (:`3`
      (bind _returnvalue_4 (`|CreateWidget` "/Game/VN_UI/BP_infolink_cutscene.BP_infolink_cutscene_C"))
      (`UserWidget.AddToViewport` _returnvalue_4 0)
      (`/Game/VN_UI/BP_infolink_cutscene.MESSAGE` _returnvalue_4 "/Game/VN_UI/Avatars/T_Infolink_Molly.T_Infolink_Molly" "Sure, but can I? I mean, wait… Why do I keep only asking questions? I feel like a plot device now." "Molly"))
    (:`4`
      (bind _returnvalue_5 (`|CreateWidget` "/Game/VN_UI/BP_infolink_cutscene.BP_infolink_cutscene_C"))
      (`UserWidget.AddToViewport` _returnvalue_5 0)
      (`/Game/VN_UI/BP_infolink_cutscene.MESSAGE` _returnvalue_5 "/Game/VN_UI/Avatars/T_Infolink_Hacker.T_Infolink_Hacker" "How inquisitive of you. No worries, sometimes one just acts like a mirror to someone else.  \nNow, I’ve banned others so no-one will see what you are doing now. Before our perp flips the switch back on, you need to sneak into a maintenance route I’ve opened.  \nThe map’s substation lies there – destroy it." "Hacker"))
    (:`5`
      ;[1 1 1] CTF1
      (bind _returnvalue_6 (`|CreateWidget` "/Game/VN_UI/BP_infolink_cutscene.BP_infolink_cutscene_C")) ; 5
      (`UserWidget.AddToViewport` _returnvalue_6 0)
      (`/Game/VN_UI/BP_infolink_cutscene.MESSAGE` _returnvalue_6 "/Game/VN_UI/Avatars/T_Infolink_Molly.T_Infolink_Molly" "So, what now?" "Molly"))
    (:`6`
      (bind _returnvalue_7 (`|CreateWidget` "/Game/VN_UI/BP_infolink_cutscene.BP_infolink_cutscene_C"))
      (`UserWidget.AddToViewport` _returnvalue_7 0)
      (`/Game/VN_UI/BP_infolink_cutscene.MESSAGE` _returnvalue_7 "/Game/VN_UI/Avatars/T_Infolink_Hacker.T_Infolink_Hacker" "Depends – you either shoot it and aid my investigation or fix it and keep this circus going. Shouldn’t be too hard to pick, since I’d be willing to help you out in return." "Hacker"))
    (:`7`
      ;;[1 0.3331 0] Comment
      (bind _returnvalue_8 (`|CreateWidget` "/Game/VN_UI/BP_infolink_cutscene.BP_infolink_cutscene_C")) ; 7 MOLLY HELPS HACKER
      (`UserWidget.AddToViewport` _returnvalue_8 0)
      (`/Game/VN_UI/BP_infolink_cutscene.MESSAGE` _returnvalue_8 "/Game/VN_UI/Avatars/T_Infolink_Hacker.T_Infolink_Hacker" "Good choice. Our necropimp should be throwing a fit any second now." "Hacker"))
    (:`8`
      (bind _returnvalue_9 (`|CreateWidget` "/Game/VN_UI/BP_infolink_cutscene.BP_infolink_cutscene_C")) ; MOLLY HELPS HACKER
      (`UserWidget.AddToViewport` _returnvalue_9 0)
      (`/Game/VN_UI/BP_infolink_cutscene.MESSAGE` _returnvalue_9 "/Game/VN_UI/Avatars/T_Infolink_Wizard.T_Infolink_Wizard" "Goddamit! Map is breaking! Ugh. Game over everyone, I’ll have to seal that one for now…" "Wizard"))
    (:`9`
      (bind _returnvalue_10 (`|CreateWidget` "/Game/VN_UI/BP_infolink_cutscene.BP_infolink_cutscene_C")) ; 9 MOLLY HELPS WIZARD
      (`UserWidget.AddToViewport` _returnvalue_10 0)
      (`/Game/VN_UI/BP_infolink_cutscene.MESSAGE` _returnvalue_10 "/Game/VN_UI/Avatars/T_Infolink_Wizard.T_Infolink_Wizard" "Oh, it fixed itself, curious. I mean – yes, it did that because I designed it that way.  \nThis map, that I built all by myself. Yes. My map." "Wizard"))))

(event `Dialogue Lobby`
  (params (Line :type Integer :default 1))
  (switch `int` Line
    (:`0`
      ;[1 1 1] LOBBY - intro
      (bind _returnvalue (`|CreateWidget` "/Game/VN_UI/BP_infolink_cutscene.BP_infolink_cutscene_C")) ; 0
      (`UserWidget.AddToViewport` _returnvalue 0)
      (`/Game/VN_UI/BP_infolink_cutscene.MESSAGE` _returnvalue "/Game/VN_UI/Avatars/T_Infolink_Molly.T_Infolink_Molly" "Hmm, something is wrong. The air feels heavy.  \nHey, Mr Wizard, you know anything about that?" "Molly"))
    (:`1`
      (bind _returnvalue_2 (`|CreateWidget` "/Game/VN_UI/BP_infolink_cutscene.BP_infolink_cutscene_C"))
      (`UserWidget.AddToViewport` _returnvalue_2 0)
      (`/Game/VN_UI/BP_infolink_cutscene.MESSAGE` _returnvalue_2 "/Game/VN_UI/Avatars/T_Infolink_Wizard.T_Infolink_Wizard" "No. The air is fine. The map is fine. The undead don’t need to breathe, so you’re good. \nNow…we are in the CTF lobby! A classic mode, revered by the gamers of old, right?  \nNow go, keeping this dimension open is an exerting task." "Wizard"))
    (:`2`
      ;[1 1 1] LOBBY - ending
      (bind _returnvalue_3 (`|CreateWidget` "/Game/VN_UI/BP_infolink_cutscene.BP_infolink_cutscene_C")) ; 2
      (`UserWidget.AddToViewport` _returnvalue_3 0)
      (`/Game/VN_UI/BP_infolink_cutscene.MESSAGE` _returnvalue_3 "/Game/VN_UI/Avatars/T_Infolink_Molly.T_Infolink_Molly" "Damn, that was close. I guess… Thanks.  \nBut how did you know how to open a dimensional rift? I thought you were some intelligence ops or a hacker." "Molly"))
    (:`3`
      (bind _returnvalue_4 (`|CreateWidget` "/Game/VN_UI/BP_infolink_cutscene.BP_infolink_cutscene_C"))
      (`UserWidget.AddToViewport` _returnvalue_4 0)
      (`/Game/VN_UI/BP_infolink_cutscene.MESSAGE` _returnvalue_4 "/Game/VN_UI/Avatars/T_Infolink_Hacker.T_Infolink_Hacker" "Well, advanced programming is indistinguishable from magic. \nYou’d be surprised how much the Occult and InfoSec branches have been cross-pollinating since we discovered [UNINTELIGIBLE]." "Hacker"))
    (:`4`
      (bind _returnvalue_5 (`|CreateWidget` "/Game/VN_UI/BP_infolink_cutscene.BP_infolink_cutscene_C"))
      (`UserWidget.AddToViewport` _returnvalue_5 0)
      (`/Game/VN_UI/BP_infolink_cutscene.MESSAGE` _returnvalue_5 "/Game/VN_UI/Avatars/T_Infolink_Hacker.T_Infolink_Hacker" "The point is, I could save you. And I have new orders – bring the Wiz and you lot to safety.  \nWe need some information – and he probably is connected to Galactamax somehow." "Hacker"))
    (:`5`
      (bind _returnvalue_6 (`|CreateWidget` "/Game/VN_UI/BP_infolink_cutscene.BP_infolink_cutscene_C"))
      (`UserWidget.AddToViewport` _returnvalue_6 0)
      (`/Game/VN_UI/BP_infolink_cutscene.MESSAGE` _returnvalue_6 "/Game/VN_UI/Avatars/T_Infolink_Molly.T_Infolink_Molly" "Some answers would be good. Ok. Let’s go then." "Molly"))))

(event `Dialogue island hacker mid`
  (params (Line :type Integer :default 1))
  (switch `int` Line
    (:`0`
      (bind _returnvalue (`|CreateWidget` "/Game/VN_UI/BP_infolink_cutscene.BP_infolink_cutscene_C"))
      (`UserWidget.AddToViewport` _returnvalue 0)
      (`/Game/VN_UI/BP_infolink_cutscene.MESSAGE` _returnvalue "/Game/VN_UI/Avatars/T_Infolink_Molly.T_Infolink_Molly" "Oh, it’s you." "Molly"))
    (:`1`
      (bind _returnvalue_2 (`|CreateWidget` "/Game/VN_UI/BP_infolink_cutscene.BP_infolink_cutscene_C"))
      (`UserWidget.AddToViewport` _returnvalue_2 0)
      (`/Game/VN_UI/BP_infolink_cutscene.MESSAGE` _returnvalue_2 "/Game/VN_UI/Avatars/T_Infolink_Hacker.T_Infolink_Hacker" " Yes. I bring dire news. This is the worst Rupture Event recorded in decades. And you?" "Hacker"))
    (:`2`
      (bind _returnvalue_3 (`|CreateWidget` "/Game/VN_UI/BP_infolink_cutscene.BP_infolink_cutscene_C"))
      (`UserWidget.AddToViewport` _returnvalue_3 0)
      (`/Game/VN_UI/BP_infolink_cutscene.MESSAGE` _returnvalue_3 "/Game/VN_UI/Avatars/T_Infolink_Molly.T_Infolink_Molly" "I have to get the blue flag – why, I don’t know. But maybe it will help us stitch the realities together. \nAt least that’s what the Wizard is thinking." "Molly"))
    (:`3`
      (bind _returnvalue_4 (`|CreateWidget` "/Game/VN_UI/BP_infolink_cutscene.BP_infolink_cutscene_C"))
      (`UserWidget.AddToViewport` _returnvalue_4 0)
      (`/Game/VN_UI/BP_infolink_cutscene.MESSAGE` _returnvalue_4 "/Game/VN_UI/Avatars/T_Infolink_Hacker.T_Infolink_Hacker" "Ok. Just watch your back. This island is not as deserted as your friend, the Wiz thought. People here… are very distrustful to outsiders. \nAnd they have been hunting undead for centuries." "Hacker"))
    (:`4`
      (bind _returnvalue_5 (`|CreateWidget` "/Game/VN_UI/BP_infolink_cutscene.BP_infolink_cutscene_C"))
      (`UserWidget.AddToViewport` _returnvalue_5 0)
      (`/Game/VN_UI/BP_infolink_cutscene.MESSAGE` _returnvalue_5 "/Game/VN_UI/Avatars/T_Infolink_Hacker.T_Infolink_Hacker" "They have perfected the weapons that just… erase the soul. Just try to stay out of sight." "Hacker"))
    (:`5`
      (bind _returnvalue_6 (`|CreateWidget` "/Game/VN_UI/BP_infolink_cutscene.BP_infolink_cutscene_C"))
      (`UserWidget.AddToViewport` _returnvalue_6 0)
      (`/Game/VN_UI/BP_infolink_cutscene.MESSAGE` _returnvalue_6 "/Game/VN_UI/Avatars/T_Infolink_Hacker.T_Infolink_Hacker" "Ok, but watch your back. This island is not as deserted as your friend, the Wiz thought. People here are… special, so to speak. \nFortunately for you, they and I go way back, so you shouldn’t encounter any problems. Just be careful." "Hacker"))))

(event `Dialogue Lab terminal`
  (params (Line :type Integer :default 1))
  (switch `int` Line
    (:`0`
      (bind _returnvalue (`|CreateWidget` "/Game/VN_UI/BP_infolink_cutscene.BP_infolink_cutscene_C"))
      (`UserWidget.AddToViewport` _returnvalue 0)
      (`/Game/VN_UI/BP_infolink_cutscene.MESSAGE` _returnvalue "/Game/VN_UI/Avatars/T_Infolink_Hacker.T_Infolink_Hacker" " All right, find the terminal for the cell block’s door controls. Helsing should be inside." "Hacker"))
    (:`1`
      (bind _returnvalue_2 (`|CreateWidget` "/Game/VN_UI/BP_infolink_cutscene.BP_infolink_cutscene_C"))
      (`UserWidget.AddToViewport` _returnvalue_2 0)
      (`/Game/VN_UI/BP_infolink_cutscene.MESSAGE` _returnvalue_2 "/Game/VN_UI/Avatars/T_Infolink_Molly.T_Infolink_Molly" "Should? Why not \"is\"?" "Molly"))
    (:`2`
      (bind _returnvalue_3 (`|CreateWidget` "/Game/VN_UI/BP_infolink_cutscene.BP_infolink_cutscene_C"))
      (`UserWidget.AddToViewport` _returnvalue_3 0)
      (`/Game/VN_UI/BP_infolink_cutscene.MESSAGE` _returnvalue_3 "/Game/VN_UI/Avatars/T_Infolink_Hacker.T_Infolink_Hacker" "Well, signal scramblers fired up the moment you entered the lab. I hope R-Frames didn’t move him somewhere else. I could shut them down and gain control of the systems if you plug in me directly." "Hacker"))
    (:`3`
      (bind _returnvalue_4 (`|CreateWidget` "/Game/VN_UI/BP_infolink_cutscene.BP_infolink_cutscene_C"))
      (`UserWidget.AddToViewport` _returnvalue_4 0)
      (`/Game/VN_UI/BP_infolink_cutscene.MESSAGE` _returnvalue_4 "/Game/VN_UI/Avatars/T_Infolink_Hacker.T_Infolink_Hacker" "Our agreement stands: you help me, you help yourself. But hey, \nit’s a free country." "Hacker"))))

(event `Lab ending portal`
  (bind _returnvalue (`|CreateWidget` "/Game/VN_UI/BP_infolink_cutscene.BP_infolink_cutscene_C"))
  (`UserWidget.AddToViewport` _returnvalue 0)
  (`/Game/VN_UI/BP_infolink_cutscene.MESSAGE` _returnvalue "/Game/VN_UI/Avatars/T_Infolink_Hacker.T_Infolink_Hacker" "Get in the rift, quick!" "Hacker"))

(fn `UserConstructionScript`)