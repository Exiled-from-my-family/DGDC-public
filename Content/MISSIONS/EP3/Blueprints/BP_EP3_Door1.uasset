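; Episode 3 mission door that starts out broken and slides open once its Open flag is set; nothing here sets that flag.
; Tick polls the flag and plays a timeline that offsets the mesh from its start location.
; A trigger box shows a broken or fixed message widget when a Character enters, re-arming on exit.
; The delayed auto-close logic is left unconnected, so the door never closes.
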(event `self.ReceiveBeginPlay`
  (set `self.DoorStartLocation` (`SceneComponent.K2_GetComponentLocation` (`self.Door_mesh`)))
  (`PrimitiveComponent.SetCollisionProfileName` (`self.Door_mesh`) "BlockAllDynamic" true))

(event `self.ReceiveTick`
  (params (DeltaSeconds :type "Float (single-precision)"))
  (if (`self.open?`)
    (`/Engine/EditorBlueprintResources/StandardMacros.DoOnce` false
      (:`Completed`
        (bind (_direction _newtrack_2) (`Timeline|DoorMovement`)
          (:`Update`
            (`self.SetTickableWhenPaused` true)
            (`SceneComponent.K2_SetWorldLocation` (`self.Door_mesh`) (+ _newtrack_2 (`self.DoorStartLocation`)) false false))
          (:`Finished`
            (`/Engine/EditorBlueprintResources/StandardMacros.DoOnce` false :!via `Reset`
              (:`Completed`
                (`GameplayStatics.PlaySoundAtLocation` "/Game/AUDIO/SFX_Doors/SC_DoorStart2.SC_DoorStart2" (`SceneComponent.K2_GetComponentLocation` (`self.Door_mesh`)) (struct) 1.0 1.0 0.0 null null null)))))))))

(event `self.TriggerBox_Player_broken.OnComponentBeginOverlap`
  (params (OverlappedComponent :type "PrimitiveComponent Object Reference") (OtherActor :type "Actor Object Reference") (OtherComp :type "PrimitiveComponent Object Reference") (OtherBodyIndex :type Integer) (bFromSweep :type Boolean) (SweepResult :type "HitResult Structure (by ref)"))
  (cast `Character` OtherActor)
  (`/Engine/EditorBlueprintResources/StandardMacros.DoOnce` false :!label _label
    (:`Completed`
      (if (`self.open?`)
        (`/Game/Blueprints/NewFunctionLibrary.clean all message widgets`)
        (`KismetSystemLibrary.Delay` 0.02)
        (bind _returnvalue (`|CreateWidget` "/Game/Blueprints/UI/UI_Pickups/UI_GenericMessage.UI_GenericMessage_C"))
        (set `/Game/Blueprints/UI/UI_Pickups/UI_GenericMessage.Message` "it' fixed now" _returnvalue)
        (`UserWidget.AddToViewport` _returnvalue 0)
        (else
          (`/Game/Blueprints/NewFunctionLibrary.clean all message widgets`)
          (`KismetSystemLibrary.Delay` 0.02)
          (bind _returnvalue_2 (`|CreateWidget` "/Game/Blueprints/UI/UI_Pickups/UI_GenericMessage.UI_GenericMessage_C"))
          (set `/Game/Blueprints/UI/UI_Pickups/UI_GenericMessage.Message` "it's broken" _returnvalue_2)
          (`UserWidget.AddToViewport` _returnvalue_2 0)
          (`KismetSystemLibrary.Delay` 3.5))))))

(event `self.TriggerBox_Player_broken.OnComponentEndOverlap`
  (params (OverlappedComponent :type "PrimitiveComponent Object Reference") (OtherActor :type "Actor Object Reference") (OtherComp :type "PrimitiveComponent Object Reference") (OtherBodyIndex :type Integer))
  (cast `Character` OtherActor)
  (goto _label :!via `Reset`))

(fn `UserConstructionScript`)