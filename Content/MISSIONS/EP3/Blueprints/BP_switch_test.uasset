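; Test power switch for Episode 3 that is meant to open BP_EP3_Door1.
; A box overlap shows a restore-power prompt and gates the Interact input, which swaps the cube's emissive material.
; Tick waits for Activated to open the door once with a pop sound, but the graph's only setter for that flag is unwired.
; Shock projectile hits on the cube just play the pop sound and reset a DoOnce.
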(event `self.ReceiveBeginPlay`)

(event `self.ReceiveTick`
  (params (DeltaSeconds :type "Float (single-precision)"))
  (if (`self.activated?`)
    (`/Engine/EditorBlueprintResources/StandardMacros.DoOnce` false
      (:`Completed`
        (`GameplayStatics.PlaySound2D` "/Game/AUDIO/SC_Pop.SC_Pop" 4.0 1.0 0.0 null null)
        (bind _returnvalue (`GameplayStatics.GetActorOfClass` "/Game/MISSIONS/EP3/Blueprints/BP_EP3_Door1.BP_EP3_Door1_C"))
        (bind _asbp_ep3_door_1 (cast `/Game/MISSIONS/EP3/Blueprints/BP_EP3_Door1` _returnvalue))
        (set `/Game/MISSIONS/EP3/Blueprints/BP_EP3_Door1.open?` true _asbp_ep3_door_1)
        (`PrimitiveComponent.SetMaterial` (`self.Cube`) 0 "/Game/kosm_fps_assets/Misc/Char_FirstPerson/Meshes/BaseMaterialEmission2.BaseMaterialEmission2")))))

(event `self.Cube.OnComponentHit`
  (params (HitComponent :type "PrimitiveComponent Object Reference") (OtherActor :type "Actor Object Reference") (OtherComp :type "PrimitiveComponent Object Reference") (NormalImpulse :type "Vector Structure") (Hit :type "HitResult Structure (by ref)"))
  (cast `/Game/Blueprints/PROJECTILES/BP_Proj_ShockinTruth` OtherActor)
  (`GameplayStatics.PlaySound2D` "/Game/AUDIO/SC_Pop.SC_Pop" 4.0 1.0 0.0 null null :!label _label)
  (`KismetSystemLibrary.Delay` 1.0)
  (`/Engine/EditorBlueprintResources/StandardMacros.DoOnce` false :!via `Reset`
    (:`Completed`
      (goto _label))))

(event `InputAction|Interact` :consume false
  (params (Key :type "Key Structure"))
  (:`Pressed`
    (`/Engine/EditorBlueprintResources/StandardMacros.Gate` true :!label _label_2
      (:`Exit`
        (`/Engine/EditorBlueprintResources/StandardMacros.DoOnce` false :!label _label_3
          (:`Completed`
            (if (and (`self.isNear?`) (not (`self.on?`)))
              (`PrimitiveComponent.SetMaterial` (`self.Cube`) 0 "/Game/kosm_fps_assets/Misc/Char_FirstPerson/Meshes/BaseMaterialEmission2.BaseMaterialEmission2")
              (else
                (set `self.on?` false :!label _label_4)))
            (`KismetSystemLibrary.Delay` 0.1)
            (goto _label_3 :!via `Reset`)))))))

(event `self.Box.OnComponentBeginOverlap`
  (params (OverlappedComponent :type "PrimitiveComponent Object Reference") (OtherActor :type "Actor Object Reference") (OtherComp :type "PrimitiveComponent Object Reference") (OtherBodyIndex :type Integer) (bFromSweep :type Boolean) (SweepResult :type "HitResult Structure (by ref)"))
  (cast `/Game/Blueprints/CHARACTERS/fpsMovementCharacter_light_1_vq3` OtherActor)
  (set `self.isNear?` true)
  (`/Game/Blueprints/NewFunctionLibrary.clean all message widgets`)
  (`KismetSystemLibrary.Delay` 0.01)
  (bind _returnvalue (`|CreateWidget` "/Game/Blueprints/UI/UI_Pickups/UI_GenericMessage.UI_GenericMessage_C" (`GameplayStatics.GetPlayerController` 0)))
  (set `/Game/Blueprints/UI/UI_Pickups/UI_GenericMessage.Message` "press 'E' to restore the power" _returnvalue)
  (`UserWidget.AddToViewport` _returnvalue 0)
  (goto _label_2 :!via `Open`))

(event `self.Box.OnComponentEndOverlap`
  (params (OverlappedComponent :type "PrimitiveComponent Object Reference") (OtherActor :type "Actor Object Reference") (OtherComp :type "PrimitiveComponent Object Reference") (OtherBodyIndex :type Integer))
  (cast `/Game/Blueprints/CHARACTERS/fpsMovementCharacter_light_1_vq3` OtherActor)
  (`|ExecutionSequence`
    (:`then_0`
      (goto _label_2 :!via `Close`))
    (:`then_1`
      (goto _label_4))))

(fn `UserConstructionScript`
  (`PrimitiveComponent.SetMaterial` (`self.Cube`) 0 "/Game/kosm_fps_assets/Misc/Char_FirstPerson/Meshes/BaseMaterialEmission.BaseMaterialEmission"))