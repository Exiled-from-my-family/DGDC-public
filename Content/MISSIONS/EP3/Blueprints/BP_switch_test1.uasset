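; BP_switch_test1 is a test switch cube for EP3 that opens a BP_EP3_Door1 when its Activated flag is true.
; Tick polls the flag and, through a DoOnce, plays a pop, sets Open on the first door found and swaps the cube's emissive material.
; ShockinTruth projectile hits only play the pop and reset a separate DoOnce after a delay; nothing here sets Activated.
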(event `self.ReceiveBeginPlay`)

(event `self.ReceiveTick`
  (params (DeltaSeconds :type "Float (single-precision)"))
  (if (`self.activated?`)
    (`/Engine/EditorBlueprintResources/StandardMacros.DoOnce` false
      (:`Completed`
        (`GameplayStatics.PlaySound2D` "/Game/AUDIO/SC_Pop.SC_Pop" 4.0 1.0 0.0 null null)
        (bind _returnvalue (`GameplayStatics.GetActorOfClass` "/Game/MISSIONS/EP3/Blueprints/BP_EP3_Door1.BP_EP3_Door1_C"))
        (bind _asbp_ep3_door_1 (cast `/Game/MISSIONS/EP3/Blueprints/BP_EP3_Door1` _returnvalue))
        (set `/Game/MISSIONS/EP3/Blueprints/BP_EP3_Door1.open?` true _asbp_ep3_door_1)
        (`PrimitiveComponent.SetMaterial` (`self.Cube`) 0 "/Game/kosm_fps_assets/Misc/Char_FirstPerson/Meshes/BaseMaterialEmission2.BaseMaterialEmission2")))))

(event `self.Cube.OnComponentHit`
  (params (HitComponent :type "PrimitiveComponent Object Reference") (OtherActor :type "Actor Object Reference") (OtherComp :type "PrimitiveComponent Object Reference") (NormalImpulse :type "Vector Structure") (Hit :type "HitResult Structure (by ref)"))
  (cast `/Game/Blueprints/PROJECTILES/BP_Proj_ShockinTruth` OtherActor)
  (`GameplayStatics.PlaySound2D` "/Game/AUDIO/SC_Pop.SC_Pop" 4.0 1.0 0.0 null null :!label _label)
  (`KismetSystemLibrary.Delay` 1.0)
  (`/Engine/EditorBlueprintResources/StandardMacros.DoOnce` false :!via `Reset`
    (:`Completed`
      (goto _label))))

(fn `UserConstructionScript`
  (`PrimitiveComponent.SetMaterial` (`self.Cube`) 0 "/Game/MATERIALS/Master/MASTER_EMISSIVE_1.MASTER_EMISSIVE_1"))