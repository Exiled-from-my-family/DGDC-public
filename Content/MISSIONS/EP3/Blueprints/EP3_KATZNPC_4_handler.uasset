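; Episode 3 NPC dialogue handler for a scripted conversation about A.M.B., GMAX and a suspect who may be Wendy.
; Talk builds the DialogSystem UI and camera angle, then Dialog switches on response EventIDs to chain lines and replies.
; The conversation forks once, with one branch playing a timed, faded cutaway to FunnyCamera.
; Both branches converge on a closing exchange that returns the view to the player character and sets Done.
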(event `self.Talk`
  (bind _dialogsystem (`/Game/AnonsDialogSystem/Blueprints/BP_DialogSystem.CreateDialogUI` :`self` (`self.DialogSystem`) :`GUITexture` "/Game/VN_UI/UI_Textures/T_Infolink_Dialogue_Flat.T_Infolink_Dialogue_Flat" :`MainSize` (1350.0 350.0) :`MainTranslation` (0.0 -25.0) :`MainBorderColor` (struct :`R` 0.300544 :`G` 0.752942 :`B` 0.491021 :`A` 1.0)))
  (bind _dialogsystem_2 (`/Game/AnonsDialogSystem/Blueprints/BP_DialogSystem.AddCameraAngle` _dialogsystem self 1.0 500.0 70.0 -50.0 true)) ; Add center angle
  (`/Game/AnonsDialogSystem/Blueprints/BP_DialogSystem.AddDialog` _dialogsystem_2 (`self.Avatar`) (`self.Name`) "..." "None" (struct :`R` 1.0 :`G` 1.0 :`B` 1.0 :`A` 1.0) (struct :`G` 0.502887 :`B` 0.250158 :`A` 1.0) (struct :`R` 1.0 :`G` 1.0 :`B` 1.0 :`A` 1.0) "/Game/kosm_fps_assets/Misc/Fonts/rexlia_rg_Font.rexlia_rg_Font" null null 0.0 0.02 (`self.Dialogue SFX`) false true)
  (bind _dialogsystem_3 (`/Game/AnonsDialogSystem/Blueprints/BP_DialogSystem.AddDialog` _dialogsystem (`self.Avatar`) (`self.Name`) "..." "None" (struct :`R` 1.0 :`G` 1.0 :`B` 1.0 :`A` 1.0) (struct :`G` 0.502887 :`B` 0.250158 :`A` 1.0) (struct :`R` 1.0 :`G` 1.0 :`B` 1.0 :`A` 1.0) "/Game/kosm_fps_assets/Misc/Fonts/rexlia_rg_Font.rexlia_rg_Font" null null 0.0 0.02 (`self.Dialogue SFX`) false true))
  (`/Game/AnonsDialogSystem/Blueprints/BP_DialogSystem.AddResponse` :`self` _dialogsystem_3 :`ResponseDialog` "Do we know who this A.M.B. person is yet?" :`EventID` "1" :`ResponseFont` "/Game/kosm_fps_assets/Misc/Fonts/rexlia_rg_Font.rexlia_rg_Font" :`TextColorHovered` (struct :`G` 1.0 :`B` 0.502887 :`A` 1.0) :`TextColorNormal` (struct :`R` 1.0 :`G` 1.0 :`B` 1.0 :`A` 1.0)))

(event `/Game/AnonsDialogSystem/Blueprints/BPI_DialogInterface.Dialog`
  (params (EventID :type Name) (SwitchID :type Integer) (DialogText :type Text))
  (`/Game/AnonsDialogSystem/Blueprints/BP_DialogSystem.GlobalDialogEvent` (`self.DialogSystem`) EventID)
  (switch `int` (`KismetStringLibrary.Conv_StringToInt` (`KismetStringLibrary.Conv_NameToString` EventID))
    (:`1`
      (bind _dialogsystem (`/Game/AnonsDialogSystem/Blueprints/BP_DialogSystem.AddDialog` (stale `self.Talk` _dialogsystem) (`self.Avatar`) (`self.Name`) "Uh... If you'd believe it, he’s joining as an athlete at GMAX casino." "None" (struct :`R` 1.0 :`G` 1.0 :`B` 1.0 :`A` 1.0) (struct :`G` 0.502887 :`B` 0.250158 :`A` 1.0) (struct :`R` 1.0 :`G` 1.0 :`B` 1.0 :`A` 1.0) "/Game/kosm_fps_assets/Misc/Fonts/rexlia_rg_Font.rexlia_rg_Font" null null 0.0 0.02 (`self.Dialogue SFX`) false true))
      (`/Game/AnonsDialogSystem/Blueprints/BP_DialogSystem.AddResponse` :`self` _dialogsystem :`ResponseDialog` "... Did they force him to be a gladiator?" :`EventID` "2" :`ResponseFont` "/Game/kosm_fps_assets/Misc/Fonts/rexlia_rg_Font.rexlia_rg_Font" :`TextColorHovered` (struct :`G` 0.715694 :`B` 1.0 :`A` 1.0) :`TextColorNormal` (struct :`R` 1.0 :`G` 1.0 :`B` 1.0 :`A` 1.0)))
    (:`2`
      (bind _dialogsystem_2 (`/Game/AnonsDialogSystem/Blueprints/BP_DialogSystem.AddDialog` (stale `self.Talk` _dialogsystem) (`self.Avatar`) (`self.Name`) "No he just joined in, the guards didn’t care." "None" (struct :`R` 1.0 :`G` 1.0 :`B` 1.0 :`A` 1.0) (struct :`G` 0.502887 :`B` 0.250158 :`A` 1.0) (struct :`R` 1.0 :`G` 1.0 :`B` 1.0 :`A` 1.0) "/Game/kosm_fps_assets/Misc/Fonts/rexlia_rg_Font.rexlia_rg_Font" null null 0.0 0.02 (`self.Dialogue SFX`) false true))
      (`/Game/AnonsDialogSystem/Blueprints/BP_DialogSystem.AddResponse` :`self` _dialogsystem_2 :`ResponseDialog` "Any other persons of interest we're supposed to be aware of?" :`EventID` "3" :`ResponseFont` "/Game/kosm_fps_assets/Misc/Fonts/rexlia_rg_Font.rexlia_rg_Font" :`TextColorHovered` (struct :`G` 0.715694 :`B` 1.0 :`A` 1.0) :`TextColorNormal` (struct :`R` 1.0 :`G` 1.0 :`B` 1.0 :`A` 1.0)))
    (:`3`
      (bind _dialogsystem_3 (`/Game/AnonsDialogSystem/Blueprints/BP_DialogSystem.AddDialog` (stale `self.Talk` _dialogsystem) (`self.Avatar`) (`self.Name`) "This girl. The same one that shared intel says is slaughtering hundreds of GMAX employees." "None" (struct :`R` 1.0 :`G` 1.0 :`B` 1.0 :`A` 1.0) (struct :`G` 0.502887 :`B` 0.250158 :`A` 1.0) (struct :`R` 1.0 :`G` 1.0 :`B` 1.0 :`A` 1.0) "/Game/kosm_fps_assets/Misc/Fonts/rexlia_rg_Font.rexlia_rg_Font" null null 0.0 0.02 (`self.Dialogue SFX`) false true))
      (bind _dialogsystem_4 (`/Game/AnonsDialogSystem/Blueprints/BP_DialogSystem.AddResponse` :`self` _dialogsystem_3 :`ResponseDialog` "Wendy? She looks like she has the same disease we have." :`EventID` "4" :`ResponseFont` "/Game/kosm_fps_assets/Misc/Fonts/rexlia_rg_Font.rexlia_rg_Font" :`TextColorHovered` (struct :`G` 0.717647 :`B` 1.0 :`A` 1.0) :`TextColorNormal` (struct :`R` 1.0 :`G` 1.0 :`B` 1.0 :`A` 1.0)))
      (`/Game/AnonsDialogSystem/Blueprints/BP_DialogSystem.AddResponse` :`self` _dialogsystem_4 :`ResponseDialog` "Killed by the hundreds by some random ghouls. Riding off of the same phenoma that’s made us sick..." :`EventID` "5" :`ResponseFont` "/Game/kosm_fps_assets/Misc/Fonts/rexlia_rg_Font.rexlia_rg_Font" :`TextColorHovered` (struct :`G` 0.717647 :`B` 1.0 :`A` 1.0) :`TextColorNormal` (struct :`R` 1.0 :`G` 1.0 :`B` 1.0 :`A` 1.0)))
    (:`4`
      (bind _dialogsystem_5 (`/Game/AnonsDialogSystem/Blueprints/BP_DialogSystem.AddDialog` (stale `self.Talk` _dialogsystem) null (`self.Name`) "She does, grayed out. Want to ask her if she's also got numbness, dryness of mouth, lack of taste, intermittent fatigue? We don't have confirmation that it's Wendy." "None" (struct :`R` 1.0 :`G` 1.0 :`B` 1.0 :`A` 1.0) (struct :`G` 0.502887 :`B` 0.250158 :`A` 1.0) (struct :`R` 1.0 :`G` 1.0 :`B` 1.0 :`A` 1.0) "/Game/kosm_fps_assets/Misc/Fonts/rexlia_rg_Font.rexlia_rg_Font" null null 0.0 0.02 null false true))
      (`/Game/AnonsDialogSystem/Blueprints/BP_DialogSystem.AddResponse` :`self` _dialogsystem_5 :`ResponseDialog` "Yeah ha sure, I'll just go chat her up. [This condition seems to serve as a massive force multiplier, are we going to get exploited?] … … I need to investigate something." :`EventID` "6" :`ResponseFont` "/Game/kosm_fps_assets/Misc/Fonts/rexlia_rg_Font.rexlia_rg_Font" :`TextColorHovered` (struct :`G` 0.715694 :`B` 1.0 :`A` 1.0) :`TextColorNormal` (struct :`R` 1.0 :`G` 1.0 :`B` 1.0 :`A` 1.0)))
    (:`5`
      (bind (_dialogsystem_6 _delayvalue) (`/Game/AnonsDialogSystem/Blueprints/BP_DialogSystem.AddDialog` (stale `self.Talk` _dialogsystem) null "Newcat" "Yeah, I think some faction of those guys don't care any more, or we're being lied to. It has got to be..." "None" (struct :`R` 1.0 :`G` 1.0 :`B` 1.0 :`A` 1.0) (struct :`G` 0.501961 :`B` 0.25098 :`A` 1.0) (struct :`R` 1.0 :`G` 1.0 :`B` 1.0 :`A` 1.0) "/Game/kosm_fps_assets/Misc/Fonts/rexlia_rg_Font.rexlia_rg_Font" null null 3.0 0.02 null false true))
      (`KismetSystemLibrary.Delay` _delayvalue)
      (`GameplayStatics.PlaySound2D` "/Game/AUDIO/SFX_Movement/SC_Dash.SC_Dash" 1.0 1.0 0.0 null null)
      (`PlayerCameraManager.StartCameraFade` (`GameplayStatics.GetPlayerCameraManager` 0) 1.0 0.0 1.0 (struct :`A` 1.0) false false)
      (`/Game/Blueprints/NewFunctionLibrary.go to actor view` (`self.funny camera`))
      (bind (_dialogsystem_7 _delayvalue_2) (`/Game/AnonsDialogSystem/Blueprints/BP_DialogSystem.AddDialog` _dialogsystem_6 (`self.Avatar`) "Newcat" "Magically stupid. \n \nIt can't be natural." "None" (struct :`R` 1.0 :`G` 1.0 :`B` 1.0 :`A` 1.0) (struct :`R` 1.0 :`B` 0.015037 :`A` 1.0) (struct :`R` 1.0 :`B` 0.006282 :`A` 1.0) "/Game/kosm_fps_assets/Misc/Fonts/rexlia_rg_Font.rexlia_rg_Font" null null 3.0 0.02 (`self.Dialogue SFX`) false true))
      (`KismetSystemLibrary.Delay` _delayvalue_2)
      (bind (_dialogsystem_8 _delayvalue_3) (`/Game/AnonsDialogSystem/Blueprints/BP_DialogSystem.AddDialog` _dialogsystem_7 null (`self.Name`) "Magical, Haven’t heard someone describe it like that." "None" (struct :`R` 1.0 :`G` 1.0 :`B` 1.0 :`A` 1.0) (struct :`G` 0.502887 :`B` 0.250158 :`A` 1.0) (struct :`R` 1.0 :`G` 1.0 :`B` 1.0 :`A` 1.0) "/Game/kosm_fps_assets/Misc/Fonts/rexlia_rg_Font.rexlia_rg_Font" null null 3.0 0.02 null false true))
      (`KismetSystemLibrary.Delay` _delayvalue_3)
      (`PlayerCameraManager.StartCameraFade` (`GameplayStatics.GetPlayerCameraManager` 0) 1.0 0.0 1.0 (struct :`A` 1.0) false false)
      (`/Game/Blueprints/NewFunctionLibrary.go to actor view` (`/Game/AnonsDialogSystem/Blueprints/BP_DialogSystem.SceneCamera` (`self.DialogSystem`)))
      (`/Game/AnonsDialogSystem/Blueprints/BP_DialogSystem.AddCameraAngle` _dialogsystem_8 self 1.0 500.0 70.0 -50.0 true) ; Add center angle
      (`/Game/AnonsDialogSystem/Blueprints/BP_DialogSystem.AddResponse` :`self` _dialogsystem_8 :`ResponseDialog` "That's obvious. Hold on… [Jealousy… Locus…  Never be…]  … I need to go on a writer’s retreat. " :`EventID` "6" :`ResponseFont` "/Game/kosm_fps_assets/Misc/Fonts/rexlia_rg_Font.rexlia_rg_Font" :`TextColorHovered` (struct :`G` 0.715694 :`B` 1.0 :`A` 1.0) :`TextColorNormal` (struct :`R` 1.0 :`G` 1.0 :`B` 1.0 :`A` 1.0)))
    (:`6`
      (bind (_dialogsystem_9 _delayvalue_4) (`/Game/AnonsDialogSystem/Blueprints/BP_DialogSystem.AddDialog` (stale `self.Talk` _dialogsystem) (`self.Avatar`) "Newcat" "[We're gonna get to the bottom of this] \n \nWho are we again?" "None" (struct :`R` 1.0 :`G` 1.0 :`B` 1.0 :`A` 1.0) (struct :`G` 0.502887 :`B` 0.250158 :`A` 1.0) (struct :`R` 1.0 :`G` 1.0 :`B` 1.0 :`A` 1.0) "/Game/kosm_fps_assets/Misc/Fonts/rexlia_rg_Font.rexlia_rg_Font" null null 2.5 0.02 (`self.Dialogue SFX`) false true)) ; 1
      (`KismetSystemLibrary.Delay` _delayvalue_4)
      (bind (_dialogsystem_10 _delayvalue_5) (`/Game/AnonsDialogSystem/Blueprints/BP_DialogSystem.AddDialog` _dialogsystem_9 null (`self.Name`) "The... Und... United... Strike Force. \nWhat could you be thinking about? Take it easy." "quit" (struct :`R` 1.0 :`G` 1.0 :`B` 1.0 :`A` 1.0) (struct :`G` 0.502887 :`B` 0.250158 :`A` 1.0) (struct :`R` 1.0 :`G` 1.0 :`B` 1.0 :`A` 1.0) "/Game/kosm_fps_assets/Misc/Fonts/rexlia_rg_Font.rexlia_rg_Font" null null 3.0 0.02 null false true)) ; 1
      (`KismetSystemLibrary.Delay` _delayvalue_5)
      (bind _outactors (`GameplayStatics.GetAllActorsOfClass` "/Game/Blueprints/CHARACTERS/fpsMovementCharacter_light_1_vq3.fpsMovementCharacter_light_1_vq3_C"))
      (`/Game/Blueprints/NewFunctionLibrary.go to actor view` (`|GetArrayItem` _outactors))
      (set `self.done` true))))

(fn `UserConstructionScript`
  (`parent.UserConstructionScript`))