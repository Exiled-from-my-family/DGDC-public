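; Episode 3 mission NPC (KATZNPC_2) that holds a short, linear conversation with Newcat about wanting to taste, feel and smell again.
; Talk builds a DialogSystem UI with an attached camera angle on the NPC, then shows the opening line and a single response.
; Dialog forwards each EventID to the global dialog event and switches on it to chain the next lines, ending on a delayed "quit" line.
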(event `self.Talk`
  (bind _dialogsystem (`/Game/AnonsDialogSystem/Blueprints/BP_DialogSystem.CreateDialogUI` :`self` (`self.DialogSystem`) :`GUITexture` "/Game/VN_UI/UI_Textures/T_Infolink_Dialogue_Flat.T_Infolink_Dialogue_Flat" :`MainSize` (1350.0 350.0) :`MainTranslation` (0.0 -25.0) :`MainBorderColor` (struct :`R` 0.300544 :`G` 0.752942 :`B` 0.491021 :`A` 1.0)))
  (bind _dialogsystem_2 (`/Game/AnonsDialogSystem/Blueprints/BP_DialogSystem.AddCameraAngle` _dialogsystem self 1.0 500.0 10.0 -50.0 true)) ; Add center angle
  (`/Game/AnonsDialogSystem/Blueprints/BP_DialogSystem.AddDialog` _dialogsystem_2 (`self.Avatar`) (`self.Name`) "... \n..." "None" (struct :`R` 1.0 :`G` 1.0 :`B` 1.0 :`A` 1.0) (struct :`G` 0.502887 :`B` 0.250158 :`A` 1.0) (struct :`R` 1.0 :`G` 1.0 :`B` 1.0 :`A` 1.0) "/Game/kosm_fps_assets/Misc/Fonts/rexlia_rg_Font.rexlia_rg_Font" null null 0.0 0.02 (`self.Dialogue SFX`) false true)
  (bind _dialogsystem_3 (`/Game/AnonsDialogSystem/Blueprints/BP_DialogSystem.AddDialog` _dialogsystem (`self.Avatar`) (`self.Name`) "... \n..." "None" (struct :`R` 1.0 :`G` 1.0 :`B` 1.0 :`A` 1.0) (struct :`G` 0.502887 :`B` 0.250158 :`A` 1.0) (struct :`R` 1.0 :`G` 1.0 :`B` 1.0 :`A` 1.0) "/Game/kosm_fps_assets/Misc/Fonts/rexlia_rg_Font.rexlia_rg_Font" null null 0.0 0.02 (`self.Dialogue SFX`) false true))
  (`/Game/AnonsDialogSystem/Blueprints/BP_DialogSystem.AddResponse` :`self` _dialogsystem_3 :`Name` "Newcat" :`ResponseDialog` "We asked this resident how he’s reacting to the recent events-" :`EventID` "1" :`ResponseFont` "/Game/kosm_fps_assets/Misc/Fonts/rexlia_rg_Font.rexlia_rg_Font" :`TextColorHovered` (struct :`G` 1.0 :`B` 0.502887 :`A` 1.0) :`TextColorNormal` (struct :`R` 1.0 :`G` 1.0 :`B` 1.0 :`A` 1.0)))

(event `/Game/AnonsDialogSystem/Blueprints/BPI_DialogInterface.Dialog`
  (params (EventID :type Name) (SwitchID :type Integer) (DialogText :type Text))
  (`/Game/AnonsDialogSystem/Blueprints/BP_DialogSystem.GlobalDialogEvent` (`self.DialogSystem`) EventID)
  (switch `int` (`KismetStringLibrary.Conv_StringToInt` (`KismetStringLibrary.Conv_NameToString` EventID))
    (:`1`
      (bind _dialogsystem (`/Game/AnonsDialogSystem/Blueprints/BP_DialogSystem.AddDialog` (stale `self.Talk` _dialogsystem) (`self.Avatar`) (`self.Name`) "I just want to taste food again, and I just want to feel again. Smell.." "None" (struct :`R` 1.0 :`G` 1.0 :`B` 1.0 :`A` 1.0) (struct :`G` 0.502887 :`B` 0.250158 :`A` 1.0) (struct :`R` 1.0 :`G` 1.0 :`B` 1.0 :`A` 1.0) "/Game/kosm_fps_assets/Misc/Fonts/rexlia_rg_Font.rexlia_rg_Font" null null 0.0 0.02 (`self.Dialogue SFX`) false true)) ; 1
      (`/Game/AnonsDialogSystem/Blueprints/BP_DialogSystem.AddResponse` :`self` _dialogsystem :`Name` "Newcat" :`ResponseDialog` "We’ll get through this soldier." :`EventID` "2" :`ResponseFont` "/Game/kosm_fps_assets/Misc/Fonts/rexlia_rg_Font.rexlia_rg_Font" :`TextColorHovered` (struct :`G` 0.715694 :`B` 1.0 :`A` 1.0) :`TextColorNormal` (struct :`R` 1.0 :`G` 1.0 :`B` 1.0 :`A` 1.0)) ; QUIT
    )
    (:`2`
      (`/Game/AnonsDialogSystem/Blueprints/BP_DialogSystem.AddDialog` (stale `self.Talk` _dialogsystem) (`self.Avatar`) (`self.Name`) "Sir... I have no doubt........." "quit" (struct :`R` 1.0 :`G` 1.0 :`B` 1.0 :`A` 1.0) (struct :`G` 0.502887 :`B` 0.250158 :`A` 1.0) (struct :`R` 1.0 :`G` 1.0 :`B` 1.0 :`A` 1.0) "/Game/kosm_fps_assets/Misc/Fonts/rexlia_rg_Font.rexlia_rg_Font" null null 2.0 0.02 (`self.Dialogue SFX`) false true) ; 1
    )))

(fn `UserConstructionScript`
  (`parent.UserConstructionScript`))