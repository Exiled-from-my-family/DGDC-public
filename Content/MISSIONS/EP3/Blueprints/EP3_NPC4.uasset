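; Episode 3 NPC Blueprint for Flak Jack, running a short branching conversation about Helsing and his returning memories.
; Talk builds the dialogue UI with a framed camera angle and first responses.
; Dialog forwards each EventID globally, then switches on it to show the next line with a new camera angle, or a quit line about finding the flag.
; Gesture calls before two branches are left unconnected.
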(event `self.Talk`
  (bind _dialogsystem (`/Game/AnonsDialogSystem/Blueprints/BP_DialogSystem.CreateDialogUI` :`self` (`self.DialogSystem`) :`GUITexture` "/Game/VN_UI/UI_Textures/T_Infolink_Dialogue_Flat.T_Infolink_Dialogue_Flat" :`MainSize` (1350.0 350.0) :`MainTranslation` (0.0 -25.0) :`MainBorderColor` (struct :`R` 0.300544 :`G` 0.752942 :`B` 0.491021 :`A` 1.0)))
  (bind _dialogsystem_2 (`/Game/AnonsDialogSystem/Blueprints/BP_DialogSystem.AddCameraAngle` _dialogsystem self 0.5 350.0 60.0 65.0 true)) ; Add center angle
  (`/Game/AnonsDialogSystem/Blueprints/BP_DialogSystem.AddDialog` _dialogsystem_2 null "Flak Jack" "Hey." "None" (struct :`R` 1.0 :`G` 1.0 :`B` 1.0 :`A` 1.0) (struct :`G` 0.502887 :`B` 0.250158 :`A` 1.0) (struct :`R` 1.0 :`G` 1.0 :`B` 1.0 :`A` 1.0) "/Game/kosm_fps_assets/Misc/Fonts/rexlia_rg_Font.rexlia_rg_Font" null null 0.0 0.02 (`self.Dialogue SFX`) false true)
  (bind _dialogsystem_3 (`/Game/AnonsDialogSystem/Blueprints/BP_DialogSystem.AddDialog` _dialogsystem null "Flak Jack" "Hey." "None" (struct :`R` 1.0 :`G` 1.0 :`B` 1.0 :`A` 1.0) (struct :`G` 0.502887 :`B` 0.250158 :`A` 1.0) (struct :`R` 1.0 :`G` 1.0 :`B` 1.0 :`A` 1.0) "/Game/kosm_fps_assets/Misc/Fonts/rexlia_rg_Font.rexlia_rg_Font" null null 0.0 0.02 (`self.Dialogue SFX`) false true))
  (bind _dialogsystem_4 (`/Game/AnonsDialogSystem/Blueprints/BP_DialogSystem.AddResponse` :`self` _dialogsystem_3 :`ResponseDialog` "Won't a fire attract unwanted attention?" :`EventID` "1" :`ResponseFont` "/Game/kosm_fps_assets/Misc/Fonts/rexlia_rg_Font.rexlia_rg_Font" :`TextColorHovered` (struct :`G` 1.0 :`B` 0.502887 :`A` 1.0) :`TextColorNormal` (struct :`R` 1.0 :`G` 1.0 :`B` 1.0 :`A` 1.0)))
  (`/Game/AnonsDialogSystem/Blueprints/BP_DialogSystem.AddResponse` :`self` _dialogsystem_4 :`ResponseDialog` "I have to go now" :`EventID` "3" :`ResponseFont` "/Game/kosm_fps_assets/Misc/Fonts/rexlia_rg_Font.rexlia_rg_Font" :`TextColorHovered` (struct :`G` 0.715694 :`B` 1.0 :`A` 1.0) :`TextColorNormal` (struct :`R` 1.0 :`G` 1.0 :`B` 1.0 :`A` 1.0)) ; QUIT
)

(event `/Game/AnonsDialogSystem/Blueprints/BPI_DialogInterface.Dialog`
  (params (EventID :type Name) (SwitchID :type Integer) (DialogText :type Text))
  (`/Game/AnonsDialogSystem/Blueprints/BP_DialogSystem.GlobalDialogEvent` (`self.DialogSystem`) EventID)
  (switch `int` (`KismetStringLibrary.Conv_StringToInt` (`KismetStringLibrary.Conv_NameToString` EventID))
    (:`1`
      (bind _dialogsystem (`/Game/AnonsDialogSystem/Blueprints/BP_DialogSystem.AddCameraAngle` (stale `self.Talk` _dialogsystem) self 1.0 400.0 60.0 40.0 true)) ; 1
      (bind _dialogsystem_2 (`/Game/AnonsDialogSystem/Blueprints/BP_DialogSystem.AddDialog` _dialogsystem null "Flak Jack" "The sun is going to set soon… If Helsing went on his own, maybe he'll see the light and reunite with the group." "None" (struct :`R` 1.0 :`G` 1.0 :`B` 1.0 :`A` 1.0) (struct :`G` 0.502887 :`B` 0.250158 :`A` 1.0) (struct :`R` 1.0 :`G` 1.0 :`B` 1.0 :`A` 1.0) "/Game/kosm_fps_assets/Misc/Fonts/rexlia_rg_Font.rexlia_rg_Font" null null 0.0 0.02 (`self.Dialogue SFX`) false true))
      (bind _dialogsystem_3 (`/Game/AnonsDialogSystem/Blueprints/BP_DialogSystem.AddResponse` :`self` _dialogsystem_2 :`ResponseDialog` "Do you think this has something to do with his memories coming back?" :`EventID` "2" :`ResponseFont` "/Game/kosm_fps_assets/Misc/Fonts/rexlia_rg_Font.rexlia_rg_Font" :`TextColorHovered` (struct :`G` 1.0 :`B` 0.502887 :`A` 1.0) :`TextColorNormal` (struct :`R` 1.0 :`G` 1.0 :`B` 1.0 :`A` 1.0)))
      (`/Game/AnonsDialogSystem/Blueprints/BP_DialogSystem.AddResponse` :`self` _dialogsystem_3 :`ResponseDialog` "I have to go now" :`EventID` "3" :`ResponseFont` "/Game/kosm_fps_assets/Misc/Fonts/rexlia_rg_Font.rexlia_rg_Font" :`TextColorHovered` (struct :`G` 0.715694 :`B` 1.0 :`A` 1.0) :`TextColorNormal` (struct :`R` 1.0 :`G` 1.0 :`B` 1.0 :`A` 1.0)) ; QUIT
    )
    (:`2`
      (bind _dialogsystem_4 (`/Game/AnonsDialogSystem/Blueprints/BP_DialogSystem.AddCameraAngle` (stale `self.Talk` _dialogsystem) self 1.2 400.0 60.0 20.0 true)) ; 2
      (bind _dialogsystem_5 (`/Game/AnonsDialogSystem/Blueprints/BP_DialogSystem.AddDialog` _dialogsystem_4 null "Flak Jack" "You saw it yourself, his… Attitude, while we were visiting that incomplete level. I have a suspicion, that place wasn't completely inside the game either." "None" (struct :`R` 1.0 :`G` 1.0 :`B` 1.0 :`A` 1.0) (struct :`G` 0.502887 :`B` 0.250158 :`A` 1.0) (struct :`R` 1.0 :`G` 1.0 :`B` 1.0 :`A` 1.0) "/Game/kosm_fps_assets/Misc/Fonts/rexlia_rg_Font.rexlia_rg_Font" null null 0.0 0.02 (`self.Dialogue SFX`) false true))
      (`/Game/AnonsDialogSystem/Blueprints/BP_DialogSystem.AddResponse` :`self` _dialogsystem_5 :`ResponseDialog` "I have to go now" :`EventID` "3" :`ResponseFont` "/Game/kosm_fps_assets/Misc/Fonts/rexlia_rg_Font.rexlia_rg_Font" :`TextColorHovered` (struct :`G` 0.715694 :`B` 1.0 :`A` 1.0) :`TextColorNormal` (struct :`R` 1.0 :`G` 1.0 :`B` 1.0 :`A` 1.0)) ; QUIT
    )
    (:`3`
      (`/Game/AnonsDialogSystem/Blueprints/BP_DialogSystem.AddDialog` (stale `self.Talk` _dialogsystem) null "Flak Jack" "Come back as soon as you find the flag." "quit" (struct :`R` 1.0 :`G` 1.0 :`B` 1.0 :`A` 1.0) (struct :`G` 0.502887 :`B` 0.250158 :`A` 1.0) (struct :`R` 1.0 :`G` 1.0 :`B` 1.0 :`A` 1.0) "/Game/kosm_fps_assets/Misc/Fonts/rexlia_rg_Font.rexlia_rg_Font" null null 0.2 0.02 (`self.Dialogue SFX`) false true) ; 3
    )))

(fn `UserConstructionScript`
  (`parent.UserConstructionScript`))