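; Episode 3 hacker interface actor that starts hidden and pops a plane in or out on APPEAR and DISAPPEAR events, playing a transmission sound.
; Timelines blend two scale lerps for a stretching open and close, and the actor hides again once the close finishes.
; When FaceThePlayer is enabled, Tick holds it ahead of and above the player and yaws it to face them.
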(event `self.ReceiveBeginPlay`
  (`self.SetActorHiddenInGame` true))

(event `APPEAR`
  (`GameplayStatics.PlaySoundAtLocation` "/Game/AUDIO/SFX_UI/SW_HackerTransmission.SW_HackerTransmission" (`self.K2_GetActorLocation`) (struct) 0.5 1.0 0.0 "/Game/kosm_fps_assets/Misc/SoundFX/SoundAttenuationNormal.SoundAttenuationNormal" null null)
  (`self.SetActorHiddenInGame` false)
  (bind (_direction _newtrack_0 _newtrack_1) (`Timeline|Timeline_0`)
    (:`Update`
      (`SceneComponent.SetRelativeScale3D` (`self.Plane`) (/ (+ (`KismetMathLibrary.VLerp` (0.5 0.0 0.0) (1.0 1.0 1.0) _newtrack_0) (`KismetMathLibrary.VLerp` (0.0 0.0 0.0) (2.0 1.0 1.0) _newtrack_1)) 2.0)))))

(event `DISAPPEAR`
  (`GameplayStatics.PlaySoundAtLocation` "/Game/AUDIO/SFX_UI/SW_HackerTransmission.SW_HackerTransmission" (`self.K2_GetActorLocation`) (struct) 0.5 1.0 0.0 "/Game/kosm_fps_assets/Misc/SoundFX/SoundAttenuationNormal.SoundAttenuationNormal" null null)
  (bind (_direction _newtrack_0 _newtrack_1) (`Timeline|Timeline_1` :!via `PlayFromStart`)
    (:`Update`
      (`SceneComponent.SetRelativeScale3D` (`self.Plane`) (/ (+ (`KismetMathLibrary.VLerp` (1.0 1.0 1.0) (0.5 0.0 0.0) _newtrack_0) (`KismetMathLibrary.VLerp` (2.0 1.0 1.0) (0.0 0.0 0.0) _newtrack_1)) 2.0)))
    (:`Finished`
      (`self.SetActorHiddenInGame` true))))

(event `self.ReceiveTick`
  (params (DeltaSeconds :type "Float (single-precision)"))
  ;[1 1 1 1 14] default set to false, so that it can only be activated for specific instances when needed
  (if (`self.face the player?`)
    (bind _player (`/Game/Blueprints/NewFunctionLibrary.get player`))
    (`SceneComponent.K2_SetWorldLocation` (`self.DefaultSceneRoot`) (+ (+ (`self.K2_GetActorLocation` _player) (0.0 0.0 200.0)) (* (`KismetMathLibrary.GetForwardVector` (`self.K2_GetActorRotation` _player)) 650.0)) false false)
    (`self.K2_SetActorRotation` (`KismetMathLibrary.MakeRotator` 0.0 0.0 (+ (.yaw (`KismetMathLibrary.FindLookAtRotation` (`self.K2_GetActorLocation`) (`self.K2_GetActorLocation` _player))) -90.0)))))

(fn `UserConstructionScript`)