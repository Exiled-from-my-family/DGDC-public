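; BP_Power_Terminal is a mission terminal the player uses to restore power.
; A box overlap by the player character shows a prompt and opens a gate for the Interact input, which marks it active, shows a confirmation, broadcasts power restored and destroys the box.
; A DAMAGED event swaps the screen to white noise and broadcasts terminal broken once, while a separate Broken flag, not set here, blocks prompt and activation.
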(event `self.ReceiveTick`
  (params (DeltaSeconds :type "Float (single-precision)")))

(event `InputAction|Interact` :consume false
  (params (Key :type "Key Structure"))
  (bind _returnvalue (`GameplayStatics.GetPlayerController` 0))
  (:`Pressed`
    (`/Engine/EditorBlueprintResources/StandardMacros.Gate` true :!label _label
      (:`Exit`
        (`/Engine/EditorBlueprintResources/StandardMacros.DoOnce` false :!label _label_2
          (:`Completed`
            (if (and (`self.IsNear?`) (not (`self.active`)) (not (`self.Broken?`)))
              (set `self.active` true)
              (`/Game/Blueprints/NewFunctionLibrary.clean all message widgets`)
              (`KismetSystemLibrary.Delay` 0.01)
              (bind _returnvalue_2 (`|CreateWidget` "/Game/Blueprints/UI/UI_Pickups/UI_GenericMessage.UI_GenericMessage_C" (`GameplayStatics.GetPlayerController` 0)))
              (set `/Game/Blueprints/UI/UI_Pickups/UI_GenericMessage.Message` "power restored" _returnvalue_2)
              (`UserWidget.AddToViewport` _returnvalue_2 0)
              (`GameplayStatics.PlaySoundAtLocation` "/Game/MISSIONS/EP3/Audio/SC_Power_On.SC_Power_On" (`self.K2_GetActorLocation`) (struct) 0.75 1.0 0.0 null null null)
              (`self.CALL_PowerRestored`)
              (`ActorComponent.K2_DestroyComponent` (`self.Box`))
              (else
                (`WidgetBlueprintLibrary.SetInputMode_GameOnly` _returnvalue :!label _label_3)
                (set `self.active` false)
                (set `PlayerController.bShowMouseCursor` false _returnvalue)
                (`/Engine/EditorBlueprintResources/StandardMacros.IsValid` null
                  (:`Is Valid`
                    (`GameplayStatics.PlaySound2D` "/Game/AUDIO/SFX_UI/SW_UI_SaveLoad.SW_UI_SaveLoad" 1.0 0.6 0.065 null null))
                  (:`Is Not Valid`
                    _))
                (`KismetSystemLibrary.Delay` 0.1)
                (goto _label_2 :!via `Reset`)))))))))

(event `self.Box.OnComponentBeginOverlap`
  (params (OverlappedComponent :type "PrimitiveComponent Object Reference") (OtherActor :type "Actor Object Reference") (OtherComp :type "PrimitiveComponent Object Reference") (OtherBodyIndex :type Integer) (bFromSweep :type Boolean) (SweepResult :type "HitResult Structure (by ref)"))
  (cast `/Game/Blueprints/CHARACTERS/fpsMovementCharacter_light_1_vq3` OtherActor)
  (set `self.IsNear?` true)
  (if (not (`self.Broken?`))
    (`/Game/Blueprints/NewFunctionLibrary.clean all message widgets`)
    (`KismetSystemLibrary.Delay` 0.01)
    (bind _returnvalue (`|CreateWidget` "/Game/Blueprints/UI/UI_Pickups/UI_GenericMessage.UI_GenericMessage_C" (`GameplayStatics.GetPlayerController` 0)))
    (set `/Game/Blueprints/UI/UI_Pickups/UI_GenericMessage.Message` (`self.Message`) _returnvalue)
    (`UserWidget.AddToViewport` _returnvalue 0)
    (goto _label :!via `Open`)))

(event `self.Box.OnComponentEndOverlap`
  (params (OverlappedComponent :type "PrimitiveComponent Object Reference") (OtherActor :type "Actor Object Reference") (OtherComp :type "PrimitiveComponent Object Reference") (OtherBodyIndex :type Integer))
  (cast `/Game/Blueprints/CHARACTERS/fpsMovementCharacter_light_1_vq3` OtherActor)
  (`|ExecutionSequence`
    (:`then_0`
      (goto _label :!via `Close`))
    (:`then_1`
      (goto _label_3))))

(event `self.SM_terminal.OnComponentHit`
  (params (HitComponent :type "PrimitiveComponent Object Reference") (OtherActor :type "Actor Object Reference") (OtherComp :type "PrimitiveComponent Object Reference") (NormalImpulse :type "Vector Structure") (Hit :type "HitResult Structure (by ref)")))

(event `DAMAGED`
  (`/Engine/EditorBlueprintResources/StandardMacros.DoOnce` false
    (:`Completed`
      (`PrimitiveComponent.SetMaterial` (`self.SM_terminal`) 1 "/Game/MATERIALS/M_WhiteNoise.M_WhiteNoise")
      (`GameplayStatics.PlaySound2D` "/Game/AUDIO/SFX_Damage/SC_Gibs_Robot.SC_Gibs_Robot" 4.0 1.0 0.0 null null)
      (`self.CALL_TerminalBroken`))))

(fn `UserConstructionScript`
  (`PrimitiveComponent.SetMaterial` (`self.SM_terminal`) 1 "/Game/MISSIONS/EP3/Meshes/Materials/M_TerminalBase1.M_TerminalBase1"))