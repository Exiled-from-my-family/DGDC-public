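; Cinematic dialogue actor for Episode 5, holding infolink conversations for story scenes such as the lab, island, caves, village chief and Helsing boss fight.
; Each scene event switches on a Line index, spawning a BP_infolink_cutscene widget with hardcoded portrait, speaker and text, skippable except in EPISODE1END.
; Quit shows the player HUD again and removes those widgets.
; Small extra events play the Hacker music and call CallSpawnLG.
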(event `SPAWN LG`
  (`self.SpawnLG`))

(event `CTF1_Hackmusic`
  (`GameplayStatics.SpawnSound2D` "/Game/MISSIONS/EP3/Music/SC_CTF1_Hacker.SC_CTF1_Hacker" 0.7 1.0 0.0 null))

(event `Quit`
  (bind _player (`/Game/Blueprints/NewFunctionLibrary.get player`))
  (`Widget.SetVisibility` (`/Game/Blueprints/CHARACTERS/fpsMovementCharacter_light_1_vq3.HUD` _player) "Visible")
  (bind _foundwidgets (`WidgetBlueprintLibrary.GetAllWidgetsOfClass` "/Game/VN_UI/BP_infolink_cutscene.BP_infolink_cutscene_C"))
  (`Widget.RemoveFromParent` _foundwidgets))

(event `Dialogue Lab helsing`
  (params (Line :type Integer :default 1))
  (switch `int` Line
    (:`0`
      (bind _returnvalue (`|CreateWidget` "/Game/VN_UI/BP_infolink_cutscene.BP_infolink_cutscene_C"))
      (`UserWidget.AddToViewport` _returnvalue 0)
      (`/Game/VN_UI/BP_infolink_cutscene.MESSAGE` _returnvalue "/Game/VN_UI/Avatars/T_Infolink_Molly.T_Infolink_Molly" "Ok. We’re fucked. I’m fucked!" "Molly"))
    (:`1`
      (bind _returnvalue_2 (`|CreateWidget` "/Game/VN_UI/BP_infolink_cutscene.BP_infolink_cutscene_C"))
      (`UserWidget.AddToViewport` _returnvalue_2 0)
      (`/Game/VN_UI/BP_infolink_cutscene.MESSAGE` _returnvalue_2 "/Game/VN_UI/Avatars/T_Infolink_Hacker.T_Infolink_Hacker" "He’s not there? I suspected as much." "Hacker"))
    (:`2`
      (bind _returnvalue_3 (`|CreateWidget` "/Game/VN_UI/BP_infolink_cutscene.BP_infolink_cutscene_C"))
      (`UserWidget.AddToViewport` _returnvalue_3 0)
      (`/Game/VN_UI/BP_infolink_cutscene.MESSAGE` _returnvalue_3 "/Game/VN_UI/Avatars/T_Infolink_Molly.T_Infolink_Molly" "Well, why didn’t you tell me? The hell am I going to do now? I’m at the bottom of a black site in the tropics, I can’t just pop out to the beach like nothing happened!" "Molly"))
    (:`3`
      (bind _returnvalue_4 (`|CreateWidget` "/Game/VN_UI/BP_infolink_cutscene.BP_infolink_cutscene_C"))
      (`UserWidget.AddToViewport` _returnvalue_4 0)
      (`/Game/VN_UI/BP_infolink_cutscene.MESSAGE` _returnvalue_4 "/Game/VN_UI/Avatars/T_Infolink_Hacker.T_Infolink_Hacker" "That might be the best thing to do right now. We have time for a quick exfil. \nUnfortunately I tripped a silent alarm. You have tangos incoming. \nBUT! I did find something interesting in one of the armories." "Hacker"))
    (:`4`
      (bind _returnvalue_5 (`|CreateWidget` "/Game/VN_UI/BP_infolink_cutscene.BP_infolink_cutscene_C"))
      (`UserWidget.AddToViewport` _returnvalue_5 0)
      (`/Game/VN_UI/BP_infolink_cutscene.MESSAGE` _returnvalue_5 "/Game/VN_UI/Avatars/T_Infolink_Hacker.T_Infolink_Hacker" "Going dark now, see you topside." "Hacker"))
    (:`5`
      (bind _returnvalue_6 (`|CreateWidget` "/Game/VN_UI/BP_infolink_cutscene.BP_infolink_cutscene_C"))
      (`UserWidget.AddToViewport` _returnvalue_6 0)
      (`/Game/VN_UI/BP_infolink_cutscene.MESSAGE` _returnvalue_6 "/Game/VN_UI/Avatars/T_Infolink_Hacker.T_Infolink_Hacker" "That might be the best thing to do right now. We have time for a quick exfil. \nUnfortunately I tripped a silent alarm. You have tangos incoming. \nTry to stay to alive. Going dark now, good luck." "Hacker"))))

(event `EPISODE 1 END`
  (params (Line :type Integer :default 1))
  (switch `int` Line
    (:`0`
      (bind _returnvalue (`|CreateWidget` "/Game/VN_UI/BP_infolink_cutscene.BP_infolink_cutscene_C" null false))
      (`UserWidget.AddToViewport` _returnvalue 0)
      (`/Game/VN_UI/BP_infolink_cutscene.MESSAGE` _returnvalue "/Game/Blueprints/DISSOLVE_VFX/Textures/Mobile/T_Noise_7_256.T_Noise_7_256" "Hello?" " "))
    (:`1`
      (bind _returnvalue_2 (`|CreateWidget` "/Game/VN_UI/BP_infolink_cutscene.BP_infolink_cutscene_C" null false))
      (`UserWidget.AddToViewport` _returnvalue_2 0)
      (`/Game/VN_UI/BP_infolink_cutscene.MESSAGE` _returnvalue_2 "/Game/Blueprints/DISSOLVE_VFX/Textures/Standart/T_Noise_8.T_Noise_8" " ...Sir? Did you receive the footage?" ""))
    (:`2`
      (bind _returnvalue_3 (`|CreateWidget` "/Game/VN_UI/BP_infolink_cutscene.BP_infolink_cutscene_C" null false))
      (`UserWidget.AddToViewport` _returnvalue_3 0)
      (`/Game/VN_UI/BP_infolink_cutscene.MESSAGE` _returnvalue_3 "/Game/Blueprints/DISSOLVE_VFX/Textures/Mobile/T_Noise_7_256.T_Noise_7_256" "Yes, I did. A sight to behold." " "))
    (:`3`
      (bind _returnvalue_4 (`|CreateWidget` "/Game/VN_UI/BP_infolink_cutscene.BP_infolink_cutscene_C" null false))
      (`UserWidget.AddToViewport` _returnvalue_4 0)
      (`/Game/VN_UI/BP_infolink_cutscene.MESSAGE` _returnvalue_4 "/Game/Blueprints/DISSOLVE_VFX/Textures/Standart/T_Noise_8.T_Noise_8" "How should we proceed? I’m at a loss." ""))
    (:`4`
      (bind _returnvalue_5 (`|CreateWidget` "/Game/VN_UI/BP_infolink_cutscene.BP_infolink_cutscene_C" null false))
      (`UserWidget.AddToViewport` _returnvalue_5 0)
      (`/Game/VN_UI/BP_infolink_cutscene.MESSAGE` _returnvalue_5 "/Game/Blueprints/DISSOLVE_VFX/Textures/Mobile/T_Noise_7_256.T_Noise_7_256" "That’s two of us then. But for different reasons." " "))
    (:`5`
      (bind _returnvalue_6 (`|CreateWidget` "/Game/VN_UI/BP_infolink_cutscene.BP_infolink_cutscene_C" null false))
      (`UserWidget.AddToViewport` _returnvalue_6 0)
      (`/Game/VN_UI/BP_infolink_cutscene.MESSAGE` _returnvalue_6 "/Game/Blueprints/DISSOLVE_VFX/Textures/Mobile/T_Noise_7_256.T_Noise_7_256" "This is going to be a long day." " "))))

(event `Helsing boss fight`
  (params (Line :type Integer :default 1))
  (switch `int` Line
    (:`0`
      (bind _returnvalue (`|CreateWidget` "/Game/VN_UI/BP_infolink_cutscene.BP_infolink_cutscene_C")) ; 0
      (`UserWidget.AddToViewport` _returnvalue 0)
      (`/Game/VN_UI/BP_infolink_cutscene.MESSAGE` _returnvalue "/Game/VN_UI/Avatars/T_Infolink_Helsing.T_Infolink_Helsing" "Were you looking for this?" "Helsing"))
    (:`1`
      (bind _returnvalue_2 (`|CreateWidget` "/Game/VN_UI/BP_infolink_cutscene.BP_infolink_cutscene_C"))
      (`UserWidget.AddToViewport` _returnvalue_2 0)
      (`/Game/VN_UI/BP_infolink_cutscene.MESSAGE` _returnvalue_2 "/Game/VN_UI/Avatars/T_Infolink_Molly.T_Infolink_Molly" "What are YOU doing here?!" "Molly"))
    (:`2`
      (bind _returnvalue_3 (`|CreateWidget` "/Game/VN_UI/BP_infolink_cutscene.BP_infolink_cutscene_C"))
      (`UserWidget.AddToViewport` _returnvalue_3 0)
      (`/Game/VN_UI/BP_infolink_cutscene.MESSAGE` _returnvalue_3 "/Game/VN_UI/Avatars/T_Infolink_Helsing.T_Infolink_Helsing" "Lucky for me, the Wizard’s ritual was indeed pretty shoddy: my memories came back. I clearly see what I have to do…again." "Helsing"))
    (:`3`
      (bind _returnvalue_4 (`|CreateWidget` "/Game/VN_UI/BP_infolink_cutscene.BP_infolink_cutscene_C"))
      (`UserWidget.AddToViewport` _returnvalue_4 0)
      (`/Game/VN_UI/BP_infolink_cutscene.MESSAGE` _returnvalue_4 "/Game/VN_UI/Avatars/T_Infolink_Molly.T_Infolink_Molly" "“Again”? You…You are the hunter!" "Molly"))
    (:`4`
      (bind _returnvalue_5 (`|CreateWidget` "/Game/VN_UI/BP_infolink_cutscene.BP_infolink_cutscene_C"))
      (`UserWidget.AddToViewport` _returnvalue_5 0)
      (`/Game/VN_UI/BP_infolink_cutscene.MESSAGE` _returnvalue_5 "/Game/VN_UI/Avatars/T_Infolink_Helsing.T_Infolink_Helsing" "I can’t let your ilk walk the earth as if nothing happened." "Helsing"))
    (:`5`
      (bind _returnvalue_6 (`|CreateWidget` "/Game/VN_UI/BP_infolink_cutscene.BP_infolink_cutscene_C"))
      (`UserWidget.AddToViewport` _returnvalue_6 0)
      (`/Game/VN_UI/BP_infolink_cutscene.MESSAGE` _returnvalue_6 "/Game/VN_UI/Avatars/T_Infolink_Molly.T_Infolink_Molly" "Banishing us all won’t solve the issue!" "Molly"))
    (:`6`
      (bind _returnvalue_7 (`|CreateWidget` "/Game/VN_UI/BP_infolink_cutscene.BP_infolink_cutscene_C"))
      (`UserWidget.AddToViewport` _returnvalue_7 0)
      (`/Game/VN_UI/BP_infolink_cutscene.MESSAGE` _returnvalue_7 "/Game/VN_UI/Avatars/T_Infolink_Helsing.T_Infolink_Helsing" "You leave me no choice, then." "Helsing"))
    (:`7`
      (bind _returnvalue_8 (`|CreateWidget` "/Game/VN_UI/BP_infolink_cutscene.BP_infolink_cutscene_C"))
      (`UserWidget.AddToViewport` _returnvalue_8 0)
      (`/Game/VN_UI/BP_infolink_cutscene.MESSAGE` _returnvalue_8 "/Game/VN_UI/Avatars/T_Infolink_Molly.T_Infolink_Molly" " I’m sorry Helsing, but you're not the hero of this story..." "Molly"))
    (:`8`
      (bind _returnvalue_9 (`|CreateWidget` "/Game/VN_UI/BP_infolink_cutscene.BP_infolink_cutscene_C"))
      (`UserWidget.AddToViewport` _returnvalue_9 0)
      (`/Game/VN_UI/BP_infolink_cutscene.MESSAGE` _returnvalue_9 "/Game/VN_UI/Avatars/T_Infolink_Helsing.T_Infolink_Helsing" "Then set me free." "Helsing"))))

(event `Dialogue Island Gmax discovery`
  (params (Line :type Integer :default 1))
  ;[1 1 1] CTF3 Gmax discovery
  (switch `int` Line
    (:`0`
      (bind _returnvalue (`|CreateWidget` "/Game/VN_UI/BP_infolink_cutscene.BP_infolink_cutscene_C")) ; 0
      (`UserWidget.AddToViewport` _returnvalue 0)
      (`/Game/VN_UI/BP_infolink_cutscene.MESSAGE` _returnvalue "/Game/VN_UI/Avatars/T_Infolink_Hacker.T_Infolink_Hacker" "Hold it, don’t go any further!" "Hacker"))
    (:`1`
      (bind _returnvalue_2 (`|CreateWidget` "/Game/VN_UI/BP_infolink_cutscene.BP_infolink_cutscene_C"))
      (`UserWidget.AddToViewport` _returnvalue_2 0)
      (`/Game/VN_UI/BP_infolink_cutscene.MESSAGE` _returnvalue_2 "/Game/VN_UI/Avatars/T_Infolink_Molly.T_Infolink_Molly" "Did not plan to. This place looks like trouble." "Molly"))
    (:`2`
      (bind _returnvalue_3 (`|CreateWidget` "/Game/VN_UI/BP_infolink_cutscene.BP_infolink_cutscene_C"))
      (`UserWidget.AddToViewport` _returnvalue_3 0)
      (`/Game/VN_UI/BP_infolink_cutscene.MESSAGE` _returnvalue_3 "/Game/VN_UI/Avatars/T_Infolink_Hacker.T_Infolink_Hacker" "Yes, this is a covert Galactamax facility." "Hacker"))
    (:`3`
      (bind _returnvalue_4 (`|CreateWidget` "/Game/VN_UI/BP_infolink_cutscene.BP_infolink_cutscene_C"))
      (`UserWidget.AddToViewport` _returnvalue_4 0)
      (`/Game/VN_UI/BP_infolink_cutscene.MESSAGE` _returnvalue_4 "/Game/VN_UI/Avatars/T_Infolink_Molly.T_Infolink_Molly" "What? Like, the billion-dollar corp? The one that started blood sports entertainment?" "Molly"))
    (:`4`
      (bind _returnvalue_5 (`|CreateWidget` "/Game/VN_UI/BP_infolink_cutscene.BP_infolink_cutscene_C"))
      (`UserWidget.AddToViewport` _returnvalue_5 0)
      (`/Game/VN_UI/BP_infolink_cutscene.MESSAGE` _returnvalue_5 "/Game/VN_UI/Avatars/T_Infolink_Hacker.T_Infolink_Hacker" "Yeah, but the name was different back then. And they had a show…" "Hacker"))
    (:`5`
      (bind _returnvalue_6 (`|CreateWidget` "/Game/VN_UI/BP_infolink_cutscene.BP_infolink_cutscene_C"))
      (`UserWidget.AddToViewport` _returnvalue_6 0)
      (`/Game/VN_UI/BP_infolink_cutscene.MESSAGE` _returnvalue_6 "/Game/VN_UI/Avatars/T_Infolink_Molly.T_Infolink_Molly" "I remember! \"Death Game”. I think one of my cousins was a fan – convicts shooting each other with stupidly big guns.  \nCan’t believe this was on the TV. It ran for a few years, right? And then it got banned." "Molly"))
    (:`6`
      (bind _returnvalue_7 (`|CreateWidget` "/Game/VN_UI/BP_infolink_cutscene.BP_infolink_cutscene_C"))
      (`UserWidget.AddToViewport` _returnvalue_7 0)
      (`/Game/VN_UI/BP_infolink_cutscene.MESSAGE` _returnvalue_7 "/Game/VN_UI/Avatars/T_Infolink_Hacker.T_Infolink_Hacker" "Bingo. It was outlawed with the Lieb/Kohn Act. The company stayed afloat though – and became Galactamax. And they could afford black sites, like this one. \nI don’t think we can handle that, there are a lot of heat signatures there, including non-human. Let’s go get that flag instead." "Hacker"))))

(event `Dialogue island part 2_1`
  (params (Line :type Integer :default 1))
  ;[1 1 1] CTF3 Part 2 -1
  (switch `int` Line
    (:`0`
      (bind _returnvalue (`|CreateWidget` "/Game/VN_UI/BP_infolink_cutscene.BP_infolink_cutscene_C")) ; 0
      (`UserWidget.AddToViewport` _returnvalue 0)
      (`/Game/VN_UI/BP_infolink_cutscene.MESSAGE` _returnvalue "/Game/VN_UI/Avatars/T_Infolink_Hacker.T_Infolink_Hacker" "Shit, they’re here. Stay low." "Hacker"))
    (:`1`
      (bind _returnvalue_2 (`|CreateWidget` "/Game/VN_UI/BP_infolink_cutscene.BP_infolink_cutscene_C"))
      (`UserWidget.AddToViewport` _returnvalue_2 0)
      (`/Game/VN_UI/BP_infolink_cutscene.MESSAGE` _returnvalue_2 "/Game/VN_UI/Avatars/T_Infolink_Galactamax.T_Infolink_Galactamax" "Control, Spear 48: Perimeter breach. Executing full response." "R-Frame"))
    (:`2`
      (bind _returnvalue_3 (`|CreateWidget` "/Game/VN_UI/BP_infolink_cutscene.BP_infolink_cutscene_C"))
      (`UserWidget.AddToViewport` _returnvalue_3 0)
      (`/Game/VN_UI/BP_infolink_cutscene.MESSAGE` _returnvalue_3 "/Game/VN_UI/Avatars/T_Infolink_MajorCommando.T_Infolink_MajorCommando" "Woah, we’re just standing here!" "Major"))
    (:`3`
      (bind _returnvalue_4 (`|CreateWidget` "/Game/VN_UI/BP_infolink_cutscene.BP_infolink_cutscene_C"))
      (`UserWidget.AddToViewport` _returnvalue_4 0)
      (`/Game/VN_UI/BP_infolink_cutscene.MESSAGE` _returnvalue_4 "/Game/VN_UI/Avatars/T_Infolink_Wizard.T_Infolink_Wizard" "Enough! I’m getting us outta here!" "Wizard"))
    (:`4`
      (bind _returnvalue_5 (`|CreateWidget` "/Game/VN_UI/BP_infolink_cutscene.BP_infolink_cutscene_C"))
      (`UserWidget.AddToViewport` _returnvalue_5 0)
      (`/Game/VN_UI/BP_infolink_cutscene.MESSAGE` _returnvalue_5 "/Game/VN_UI/Avatars/T_Infolink_Rumbletron.T_Infolink_Rumbletron" "Wait! What about [Molly, Molly, Mo-] and the [Vampire Savior]?" "Rumbletron"))
    (:`5`
      (bind _returnvalue_6 (`|CreateWidget` "/Game/VN_UI/BP_infolink_cutscene.BP_infolink_cutscene_C"))
      (`UserWidget.AddToViewport` _returnvalue_6 0)
      (`/Game/VN_UI/BP_infolink_cutscene.MESSAGE` _returnvalue_6 "/Game/VN_UI/Avatars/T_Infolink_Galactamax.T_Infolink_Galactamax" "Target lost. Sweep and resume." "R-Frame"))
    (:`6`
      (bind _returnvalue_7 (`|CreateWidget` "/Game/VN_UI/BP_infolink_cutscene.BP_infolink_cutscene_C"))
      (`UserWidget.AddToViewport` _returnvalue_7 0)
      (`/Game/VN_UI/BP_infolink_cutscene.MESSAGE` _returnvalue_7 "/Game/VN_UI/Avatars/T_Infolink_Hacker.T_Infolink_Hacker" "Hide, quick! And don’t move!" "Hacker"))))

(event `Dialogues Chief intro`
  (params (Line :type Integer :default 1))
  (switch `int` Line
    (:`0`
      ;[1 1 1] VILLAGE CHIEF INTRO
      (bind _returnvalue (`|CreateWidget` "/Game/VN_UI/BP_infolink_cutscene.BP_infolink_cutscene_C")) ; 0
      (`UserWidget.AddToViewport` _returnvalue 0)
      (`/Game/VN_UI/BP_infolink_cutscene.MESSAGE` _returnvalue "/Game/VN_UI/Avatars/T_Infolink_ChiefNative.T_Infolink_ChiefNative" "So, you must be the lost soul that has been causing all this racket. Welcome to my village, our mutual friend has already told me everything: you're looking for a way out of here, aren't you?" "Chief"))
    (:`1`
      (bind _returnvalue_2 (`|CreateWidget` "/Game/VN_UI/BP_infolink_cutscene.BP_infolink_cutscene_C"))
      (`UserWidget.AddToViewport` _returnvalue_2 0)
      (`/Game/VN_UI/BP_infolink_cutscene.MESSAGE` _returnvalue_2 "/Game/VN_UI/Avatars/T_Infolink_Molly.T_Infolink_Molly" "Indeed, could you help me out with that?" "Molly"))
    (:`2`
      (bind _returnvalue_3 (`|CreateWidget` "/Game/VN_UI/BP_infolink_cutscene.BP_infolink_cutscene_C"))
      (`UserWidget.AddToViewport` _returnvalue_3 0)
      (`/Game/VN_UI/BP_infolink_cutscene.MESSAGE` _returnvalue_3 "/Game/VN_UI/Avatars/T_Infolink_ChiefNative.T_Infolink_ChiefNative" "Absolutely. Creating a passage to your final destination should be possible, but I'll need you to gather your companions before we can go through with it: I don't think I'd be able to open more than one in such a short notice." "Chief"))
    (:`3`
      (bind _returnvalue_4 (`|CreateWidget` "/Game/VN_UI/BP_infolink_cutscene.BP_infolink_cutscene_C"))
      (`UserWidget.AddToViewport` _returnvalue_4 0)
      (`/Game/VN_UI/BP_infolink_cutscene.MESSAGE` _returnvalue_4 "/Game/VN_UI/Avatars/T_Infolink_Molly.T_Infolink_Molly" "I'll just go pick'em up while you do your preparations, if you tell me where I should start looking." "Molly"))
    (:`4`
      (bind _returnvalue_5 (`|CreateWidget` "/Game/VN_UI/BP_infolink_cutscene.BP_infolink_cutscene_C"))
      (`UserWidget.AddToViewport` _returnvalue_5 0)
      (`/Game/VN_UI/BP_infolink_cutscene.MESSAGE` _returnvalue_5 "/Game/VN_UI/Avatars/T_Infolink_ChiefNative.T_Infolink_ChiefNative" "Ah yes, your \"Hacker\" friend did bring that up. They're currently held captive in a Galactamax facility, locked inside a virtual dimension isolated from the rest of Galactamax's network. If you stole the physical drive containing it and brought it here, me and our \"Hacker\" friend could devise a way to extract them from it." "Chief"))
    (:`5`
      (bind _returnvalue_6 (`|CreateWidget` "/Game/VN_UI/BP_infolink_cutscene.BP_infolink_cutscene_C"))
      (`UserWidget.AddToViewport` _returnvalue_6 0)
      (`/Game/VN_UI/BP_infolink_cutscene.MESSAGE` _returnvalue_6 "/Game/VN_UI/Avatars/T_Infolink_Molly.T_Infolink_Molly" "Sounds good,  how do I get there?" "Molly"))
    (:`6`
      (bind _returnvalue_7 (`|CreateWidget` "/Game/VN_UI/BP_infolink_cutscene.BP_infolink_cutscene_C"))
      (`UserWidget.AddToViewport` _returnvalue_7 0)
      (`/Game/VN_UI/BP_infolink_cutscene.MESSAGE` _returnvalue_7 "/Game/VN_UI/Avatars/T_Infolink_ChiefNative.T_Infolink_ChiefNative" "Back when they first came here, the Galactamax researchers stumbled into our tunnel network while digging their own. They thought they had closed the passage after that, but we dug a secondary one just in case: you should be able to access it by going back to the catacombs whence you came and looking for a tunnel blocked by a guard. I'll tell him to let you through right away." "Chief"))
    (:`7`
      (bind _returnvalue_8 (`|CreateWidget` "/Game/VN_UI/BP_infolink_cutscene.BP_infolink_cutscene_C"))
      (`UserWidget.AddToViewport` _returnvalue_8 0)
      (`/Game/VN_UI/BP_infolink_cutscene.MESSAGE` _returnvalue_8 "/Game/VN_UI/Avatars/T_Infolink_Molly.T_Infolink_Molly" "Thank you." "Molly"))
    (:`8`
      (bind _returnvalue_9 (`|CreateWidget` "/Game/VN_UI/BP_infolink_cutscene.BP_infolink_cutscene_C"))
      (`UserWidget.AddToViewport` _returnvalue_9 0)
      (`/Game/VN_UI/BP_infolink_cutscene.MESSAGE` _returnvalue_9 "/Game/VN_UI/Avatars/T_Infolink_ChiefNative.T_Infolink_ChiefNative" "Good hunting." "Chief"))))

(event `Dialogue caves intro`
  (params (Line :type Integer :default 1))
  (switch `int` Line
    (:`0`
      ;[1 1 1] CAVES HUB INTRO
      (bind _returnvalue (`|CreateWidget` "/Game/VN_UI/BP_infolink_cutscene.BP_infolink_cutscene_C"))
      (`UserWidget.AddToViewport` _returnvalue 0)
      (`/Game/VN_UI/BP_infolink_cutscene.MESSAGE` _returnvalue "/Game/VN_UI/Avatars/T_Infolink_Molly.T_Infolink_Molly" "I’m surprised you could set up another portal on such a short notice." "Molly"))
    (:`1`
      (bind _returnvalue_2 (`|CreateWidget` "/Game/VN_UI/BP_infolink_cutscene.BP_infolink_cutscene_C"))
      (`UserWidget.AddToViewport` _returnvalue_2 0)
      (`/Game/VN_UI/BP_infolink_cutscene.MESSAGE` _returnvalue_2 "/Game/VN_UI/Avatars/T_Infolink_Hacker.T_Infolink_Hacker" "Time doesn’t flow at the same rate inside the simulation as it does in the real world. Now let’s focus on the present. I managed to hack inside the test program that was being run by the Gmax researchers." "Hacker"))
    (:`2`
      (bind _returnvalue_3 (`|CreateWidget` "/Game/VN_UI/BP_infolink_cutscene.BP_infolink_cutscene_C"))
      (`UserWidget.AddToViewport` _returnvalue_3 0)
      (`/Game/VN_UI/BP_infolink_cutscene.MESSAGE` _returnvalue_3 "/Game/VN_UI/Avatars/T_Infolink_Hacker.T_Infolink_Hacker" "The virtual casino is now unreachable by Galactamax, and it works like any other lobby you visited so far." "Hacker"))
    (:`3`
      (bind _returnvalue_4 (`|CreateWidget` "/Game/VN_UI/BP_infolink_cutscene.BP_infolink_cutscene_C"))
      (`UserWidget.AddToViewport` _returnvalue_4 0)
      (`/Game/VN_UI/BP_infolink_cutscene.MESSAGE` _returnvalue_4 "/Game/VN_UI/Avatars/T_Infolink_Molly.T_Infolink_Molly" "If we were safe there then why did you bring me here, wherever “here” is." "Molly"))
    (:`4`
      (bind _returnvalue_5 (`|CreateWidget` "/Game/VN_UI/BP_infolink_cutscene.BP_infolink_cutscene_C"))
      (`UserWidget.AddToViewport` _returnvalue_5 0)
      (`/Game/VN_UI/BP_infolink_cutscene.MESSAGE` _returnvalue_5 "/Game/VN_UI/Avatars/T_Infolink_Hacker.T_Infolink_Hacker" "We’re below the Island. Remember when I told you that me and the natives go way back?" "Hacker"))
    (:`5`
      (bind _returnvalue_6 (`|CreateWidget` "/Game/VN_UI/BP_infolink_cutscene.BP_infolink_cutscene_C"))
      (`UserWidget.AddToViewport` _returnvalue_6 0)
      (`/Game/VN_UI/BP_infolink_cutscene.MESSAGE` _returnvalue_6 "/Game/VN_UI/Avatars/T_Infolink_Hacker.T_Infolink_Hacker" "You’re inside the inner part of the dominion they guard. I want you to meet someone." "Hacker"))))

(event `Dialogue Lobby`
  (params (Line :type Integer :default 1))
  (switch `int` Line
    (:`0`
      ;[1 1 1] LOBBY - intro
      (bind _returnvalue (`|CreateWidget` "/Game/VN_UI/BP_infolink_cutscene.BP_infolink_cutscene_C")) ; 0
      (`UserWidget.AddToViewport` _returnvalue 0)
      (`/Game/VN_UI/BP_infolink_cutscene.MESSAGE` _returnvalue "/Game/VN_UI/Avatars/T_Infolink_Molly.T_Infolink_Molly" "Hmm, something is wrong. The air feels heavy.  \nHey, Mr Wizard, you know anything about that?" "Molly"))
    (:`1`
      (bind _returnvalue_2 (`|CreateWidget` "/Game/VN_UI/BP_infolink_cutscene.BP_infolink_cutscene_C"))
      (`UserWidget.AddToViewport` _returnvalue_2 0)
      (`/Game/VN_UI/BP_infolink_cutscene.MESSAGE` _returnvalue_2 "/Game/VN_UI/Avatars/T_Infolink_Wizard.T_Infolink_Wizard" "No. The air is fine. The map is fine. The undead don’t need to breathe, so you’re good. \nNow…we are in the CTF lobby! A classic mode, revered by the gamers of old, right?  \nNow go, keeping this dimension open is an exerting task." "Wizard"))
    (:`2`
      ;[1 1 1] LOBBY - ending
      (bind _returnvalue_3 (`|CreateWidget` "/Game/VN_UI/BP_infolink_cutscene.BP_infolink_cutscene_C")) ; 2
      (`UserWidget.AddToViewport` _returnvalue_3 0)
      (`/Game/VN_UI/BP_infolink_cutscene.MESSAGE` _returnvalue_3 "/Game/VN_UI/Avatars/T_Infolink_Molly.T_Infolink_Molly" "Damn, that was close. I guess… Thanks.  \nBut how did you know how to open a dimensional rift? I thought you were some intelligence ops or a hacker." "Molly"))
    (:`3`
      (bind _returnvalue_4 (`|CreateWidget` "/Game/VN_UI/BP_infolink_cutscene.BP_infolink_cutscene_C"))
      (`UserWidget.AddToViewport` _returnvalue_4 0)
      (`/Game/VN_UI/BP_infolink_cutscene.MESSAGE` _returnvalue_4 "/Game/VN_UI/Avatars/T_Infolink_Hacker.T_Infolink_Hacker" "Well, advanced programming is indistinguishable from magic. \nYou’d be surprised how much the Occult and InfoSec branches have been cross-pollinating since we discovered [UNINTELIGIBLE]." "Hacker"))
    (:`4`
      (bind _returnvalue_5 (`|CreateWidget` "/Game/VN_UI/BP_infolink_cutscene.BP_infolink_cutscene_C"))
      (`UserWidget.AddToViewport` _returnvalue_5 0)
      (`/Game/VN_UI/BP_infolink_cutscene.MESSAGE` _returnvalue_5 "/Game/VN_UI/Avatars/T_Infolink_Hacker.T_Infolink_Hacker" "The point is, I could save you. And I have new orders – bring the Wiz and you lot to safety.  \nWe need some information – and he probably is connected to Galactamax somehow." "Hacker"))
    (:`5`
      (bind _returnvalue_6 (`|CreateWidget` "/Game/VN_UI/BP_infolink_cutscene.BP_infolink_cutscene_C"))
      (`UserWidget.AddToViewport` _returnvalue_6 0)
      (`/Game/VN_UI/BP_infolink_cutscene.MESSAGE` _returnvalue_6 "/Game/VN_UI/Avatars/T_Infolink_Molly.T_Infolink_Molly" "Some answers would be good. Ok. Let’s go then." "Molly"))))

(event `Mountai dude intro`
  (params (Line :type Integer :default 1))
  (switch `int` Line
    (:`0`
      ;[1 1 1] MOUNTAIN ENTITY
      (bind _returnvalue (`|CreateWidget` "/Game/VN_UI/BP_infolink_cutscene.BP_infolink_cutscene_C"))
      (`UserWidget.AddToViewport` _returnvalue 0)
      (`/Game/VN_UI/BP_infolink_cutscene.MESSAGE` _returnvalue "/Game/VN_UI/Avatars/T_Infolink_Molly.T_Infolink_Molly" "Is this another one of your tricks?" "Molly"))
    (:`1`
      (bind _returnvalue_2 (`|CreateWidget` "/Game/VN_UI/BP_infolink_cutscene.BP_infolink_cutscene_C"))
      (`UserWidget.AddToViewport` _returnvalue_2 0)
      (`/Game/VN_UI/BP_infolink_cutscene.MESSAGE` _returnvalue_2 "/Game/VN_UI/Avatars/T_Infolink_Mountain.T_Infolink_Mountain" "At last, You brought her to me." "Mountain Entity"))
    (:`2`
      (bind _returnvalue_3 (`|CreateWidget` "/Game/VN_UI/BP_infolink_cutscene.BP_infolink_cutscene_C"))
      (`UserWidget.AddToViewport` _returnvalue_3 0)
      (`/Game/VN_UI/BP_infolink_cutscene.MESSAGE` _returnvalue_3 "/Game/VN_UI/Avatars/T_Infolink_Hacker.T_Infolink_Hacker" "The outside world is in danger; someone interfered with the natural order and your knowledge would be extraordinarily useful. Please, help us." "Hacker"))
    (:`3`
      (bind _returnvalue_4 (`|CreateWidget` "/Game/VN_UI/BP_infolink_cutscene.BP_infolink_cutscene_C"))
      (`UserWidget.AddToViewport` _returnvalue_4 0)
      (`/Game/VN_UI/BP_infolink_cutscene.MESSAGE` _returnvalue_4 "/Game/VN_UI/Avatars/T_Infolink_Mountain.T_Infolink_Mountain" "Behind this door lies a weapon that hasn’t been used for centuries: it was conjured a long, long time ago, in a magical world." "Mountain Entity"))
    (:`4`
      (bind _returnvalue_5 (`|CreateWidget` "/Game/VN_UI/BP_infolink_cutscene.BP_infolink_cutscene_C"))
      (`UserWidget.AddToViewport` _returnvalue_5 0)
      (`/Game/VN_UI/BP_infolink_cutscene.MESSAGE` _returnvalue_5 "/Game/VN_UI/Avatars/T_Infolink_Mountain.T_Infolink_Mountain" "A hunter from another land was the first who recognized the dangers of the place I inhabit, and together we forged The Hammer, so that whenever the underworld would leak into the living reality one could…solve that problem." "Mountain Entity"))
    (:`5`
      (bind _returnvalue_6 (`|CreateWidget` "/Game/VN_UI/BP_infolink_cutscene.BP_infolink_cutscene_C"))
      (`UserWidget.AddToViewport` _returnvalue_6 0)
      (`/Game/VN_UI/BP_infolink_cutscene.MESSAGE` _returnvalue_6 "/Game/VN_UI/Avatars/T_Infolink_Mountain.T_Infolink_Mountain" "Go forth, and prove yourself to be worthy of wielding The Hammer." "Mountain Entity"))
    (:`6`
      ;;[1 0.2505 0] AFTER HAMMER
      (bind _returnvalue_7 (`|CreateWidget` "/Game/VN_UI/BP_infolink_cutscene.BP_infolink_cutscene_C"))
      (`UserWidget.AddToViewport` _returnvalue_7 0)
      (`/Game/VN_UI/BP_infolink_cutscene.MESSAGE` _returnvalue_7 "/Game/VN_UI/Avatars/T_Infolink_Mountain.T_Infolink_Mountain" "You have proven yourself worthy. Good. You are now free to leave this place." "Mountain Entity"))
    (:`7`
      (bind _returnvalue_8 (`|CreateWidget` "/Game/VN_UI/BP_infolink_cutscene.BP_infolink_cutscene_C"))
      (`UserWidget.AddToViewport` _returnvalue_8 0)
      (`/Game/VN_UI/BP_infolink_cutscene.MESSAGE` _returnvalue_8 "/Game/VN_UI/Avatars/T_Infolink_Hacker.T_Infolink_Hacker" "There's a passage here that leads to one of the Islanders’ villages: my contact is there." "Hacker"))))

(event `Dialogue island hacker mid`
  (params (Line :type Integer :default 1))
  (switch `int` Line
    (:`0`
      (bind _returnvalue (`|CreateWidget` "/Game/VN_UI/BP_infolink_cutscene.BP_infolink_cutscene_C"))
      (`UserWidget.AddToViewport` _returnvalue 0)
      (`/Game/VN_UI/BP_infolink_cutscene.MESSAGE` _returnvalue "/Game/VN_UI/Avatars/T_Infolink_Molly.T_Infolink_Molly" "Oh, it’s you." "Molly"))
    (:`1`
      (bind _returnvalue_2 (`|CreateWidget` "/Game/VN_UI/BP_infolink_cutscene.BP_infolink_cutscene_C"))
      (`UserWidget.AddToViewport` _returnvalue_2 0)
      (`/Game/VN_UI/BP_infolink_cutscene.MESSAGE` _returnvalue_2 "/Game/VN_UI/Avatars/T_Infolink_Hacker.T_Infolink_Hacker" " Yes. I bring dire news. This is the worst Rupture Event recorded in decades. And you?" "Hacker"))
    (:`2`
      (bind _returnvalue_3 (`|CreateWidget` "/Game/VN_UI/BP_infolink_cutscene.BP_infolink_cutscene_C"))
      (`UserWidget.AddToViewport` _returnvalue_3 0)
      (`/Game/VN_UI/BP_infolink_cutscene.MESSAGE` _returnvalue_3 "/Game/VN_UI/Avatars/T_Infolink_Molly.T_Infolink_Molly" "I have to get the blue flag – why, I don’t know. But maybe it will help us stitch the realities together. \nAt least that’s what the Wizard is thinking." "Molly"))
    (:`3`
      (bind _returnvalue_4 (`|CreateWidget` "/Game/VN_UI/BP_infolink_cutscene.BP_infolink_cutscene_C"))
      (`UserWidget.AddToViewport` _returnvalue_4 0)
      (`/Game/VN_UI/BP_infolink_cutscene.MESSAGE` _returnvalue_4 "/Game/VN_UI/Avatars/T_Infolink_Hacker.T_Infolink_Hacker" "Ok. Just watch your back. This island is not as deserted as your friend, the Wiz thought. People here… are very distrustful to outsiders. \nAnd they have been hunting undead for centuries." "Hacker"))
    (:`4`
      (bind _returnvalue_5 (`|CreateWidget` "/Game/VN_UI/BP_infolink_cutscene.BP_infolink_cutscene_C"))
      (`UserWidget.AddToViewport` _returnvalue_5 0)
      (`/Game/VN_UI/BP_infolink_cutscene.MESSAGE` _returnvalue_5 "/Game/VN_UI/Avatars/T_Infolink_Hacker.T_Infolink_Hacker" "They have perfected the weapons that just… erase the soul. Just try to stay out of sight." "Hacker"))
    (:`5`
      (bind _returnvalue_6 (`|CreateWidget` "/Game/VN_UI/BP_infolink_cutscene.BP_infolink_cutscene_C"))
      (`UserWidget.AddToViewport` _returnvalue_6 0)
      (`/Game/VN_UI/BP_infolink_cutscene.MESSAGE` _returnvalue_6 "/Game/VN_UI/Avatars/T_Infolink_Hacker.T_Infolink_Hacker" "Ok, but watch your back. This island is not as deserted as your friend, the Wiz thought. People here are… special, so to speak. \nFortunately for you, they and I go way back, so you shouldn’t encounter any problems. Just be careful." "Hacker"))))

(event `Dialogue Lab terminal`
  (params (Line :type Integer :default 1))
  (switch `int` Line
    (:`0`
      (bind _returnvalue (`|CreateWidget` "/Game/VN_UI/BP_infolink_cutscene.BP_infolink_cutscene_C"))
      (`UserWidget.AddToViewport` _returnvalue 0)
      (`/Game/VN_UI/BP_infolink_cutscene.MESSAGE` _returnvalue "/Game/VN_UI/Avatars/T_Infolink_Hacker.T_Infolink_Hacker" " All right, find the terminal for the cell block’s door controls. Helsing should be inside." "Hacker"))
    (:`1`
      (bind _returnvalue_2 (`|CreateWidget` "/Game/VN_UI/BP_infolink_cutscene.BP_infolink_cutscene_C"))
      (`UserWidget.AddToViewport` _returnvalue_2 0)
      (`/Game/VN_UI/BP_infolink_cutscene.MESSAGE` _returnvalue_2 "/Game/VN_UI/Avatars/T_Infolink_Molly.T_Infolink_Molly" "Should? Why not \"is\"?" "Molly"))
    (:`2`
      (bind _returnvalue_3 (`|CreateWidget` "/Game/VN_UI/BP_infolink_cutscene.BP_infolink_cutscene_C"))
      (`UserWidget.AddToViewport` _returnvalue_3 0)
      (`/Game/VN_UI/BP_infolink_cutscene.MESSAGE` _returnvalue_3 "/Game/VN_UI/Avatars/T_Infolink_Hacker.T_Infolink_Hacker" "Well, signal scramblers fired up the moment you entered the lab. I hope R-Frames didn’t move him somewhere else. I could shut them down and gain control of the systems if you plug in me directly." "Hacker"))
    (:`3`
      (bind _returnvalue_4 (`|CreateWidget` "/Game/VN_UI/BP_infolink_cutscene.BP_infolink_cutscene_C"))
      (`UserWidget.AddToViewport` _returnvalue_4 0)
      (`/Game/VN_UI/BP_infolink_cutscene.MESSAGE` _returnvalue_4 "/Game/VN_UI/Avatars/T_Infolink_Hacker.T_Infolink_Hacker" "Our agreement stands: you help me, you help yourself. But hey, \nit’s a free country." "Hacker"))))

(event `Lab ending portal`
  (bind _returnvalue (`|CreateWidget` "/Game/VN_UI/BP_infolink_cutscene.BP_infolink_cutscene_C"))
  (`UserWidget.AddToViewport` _returnvalue 0)
  (`/Game/VN_UI/BP_infolink_cutscene.MESSAGE` _returnvalue "/Game/VN_UI/Avatars/T_Infolink_Hacker.T_Infolink_Hacker" "Get in the rift, quick!" "Hacker"))

(fn `UserConstructionScript`)