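; BP_GiantGrid procedurally builds a giant 3D lattice of stretched static mesh bars, sized by X, Y and Z counts.
; Buildgrid uses nested loops to add long bars, alternating rotation and spacing by Y-index parity, plus a very tall vertical bar for each X/Y pair.
; The construction script builds it on the one-shot BUILD toggle or persistent PermBUILD, while HideInEditor defers building to BeginPlay.
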(event `self.ReceiveBeginPlay`
  (if (`self.Hide in editor`)
    (`self.buildgrid`)))

(fn `buildgrid`
  (bind _z (`self.z`))
  (for _index (range (+ (`self.x`) 1))
    (for _index_2 (range (+ (`self.y`) 1))
      (for _index_3 (range (+ _z 1))
        (bind _returnvalue (* _index 800.0))
        (bind _returnvalue_2 (`KismetMathLibrary.Conv_IntToBool` (mod _index_2 2)))
        (bind _returnvalue_3 (* _index_2 (`KismetMathLibrary.SelectFloat` 800.0 400.0 _returnvalue_2)))
        (`AddComponent|NODE_AddStaticMeshComponent-0` :`RelativeTransform` (`KismetMathLibrary.MakeTransform` (`KismetMathLibrary.MakeVector` _returnvalue _returnvalue_3 (* _index_3 800.0)) (`KismetMathLibrary.SelectRotator` (struct) (struct :`Yaw` 90.0) _returnvalue_2) (0.1 100.0 0.1))))
      (`AddComponent|NODE_AddStaticMeshComponent-1` :`RelativeTransform` (`KismetMathLibrary.MakeTransform` (`KismetMathLibrary.MakeVector` _returnvalue _returnvalue_3 (* (/ _z 2) 800.0)) (struct) (0.1 0.1 9001.0))))))

(fn `UserConstructionScript`
  (if (`self.Hide in editor`)
    _
    (elif (or (`self.BUILD`) (`self.perm BUILD`))
      (`self.buildgrid`)
      (set `self.BUILD` false))))