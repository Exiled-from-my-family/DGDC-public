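; Episode 5 gate guard NPC that tells the player the gate opens only from the other side and hints at danger beyond.
; Talk builds the DialogSystem UI with a camera angle attached to the guard, then adds the opening line and responses.
; Dialog forwards each EventID to GlobalDialogEvent, then switches on it to play gestures, add follow-up lines or quit.
; The outpost and Chief branch (ID 4) has no response leading to it here.
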(event `self.Talk`
  (bind _dialogsystem (`/Game/AnonsDialogSystem/Blueprints/BP_DialogSystem.CreateDialogUI` :`self` (`self.DialogSystem`) :`GUITexture` "/Game/VN_UI/UI_Textures/T_Infolink_Dialogue_Flat.T_Infolink_Dialogue_Flat" :`MainSize` (1350.0 350.0) :`MainTranslation` (0.0 -25.0) :`MainBorderColor` (struct :`R` 0.300544 :`G` 0.752942 :`B` 0.491021 :`A` 1.0)))
  (`/Game/AnonsDialogSystem/Blueprints/BP_DialogSystem.AddCameraAngle` _dialogsystem self 0.5 450.0 30.0 35.0 true) ; Add center angle
  (bind _dialogsystem_2 (`/Game/AnonsDialogSystem/Blueprints/BP_DialogSystem.AddDialog` _dialogsystem null "Guard" "Gate's closed." "None" (struct :`R` 1.0 :`G` 1.0 :`B` 1.0 :`A` 1.0) (struct :`G` 0.502887 :`B` 0.250158 :`A` 1.0) (struct :`R` 1.0 :`G` 1.0 :`B` 1.0 :`A` 1.0) "/Game/kosm_fps_assets/Misc/Fonts/rexlia_rg_Font.rexlia_rg_Font" null null 0.0 0.02 (`self.Dialogue SFX`) false true))
  (bind _dialogsystem_3 (`/Game/AnonsDialogSystem/Blueprints/BP_DialogSystem.AddResponse` :`self` _dialogsystem_2 :`ResponseDialog` "How do I get through?" :`EventID` "1" :`ResponseFont` "/Game/kosm_fps_assets/Misc/Fonts/rexlia_rg_Font.rexlia_rg_Font" :`TextColorHovered` (struct :`G` 1.0 :`B` 0.502887 :`A` 1.0) :`TextColorNormal` (struct :`R` 1.0 :`G` 1.0 :`B` 1.0 :`A` 1.0)))
  (bind _dialogsystem_4 (`/Game/AnonsDialogSystem/Blueprints/BP_DialogSystem.AddResponse` :`self` _dialogsystem_3 :`ResponseDialog` "What's behind it?" :`EventID` "2" :`ResponseFont` "/Game/kosm_fps_assets/Misc/Fonts/rexlia_rg_Font.rexlia_rg_Font" :`TextColorHovered` (struct :`G` 1.0 :`B` 0.502887 :`A` 1.0) :`TextColorNormal` (struct :`R` 1.0 :`G` 1.0 :`B` 1.0 :`A` 1.0)))
  (`/Game/AnonsDialogSystem/Blueprints/BP_DialogSystem.AddResponse` :`self` _dialogsystem_4 :`ResponseDialog` "I have to go now" :`EventID` "5" :`ResponseFont` "/Game/kosm_fps_assets/Misc/Fonts/rexlia_rg_Font.rexlia_rg_Font" :`TextColorHovered` (struct :`G` 0.715694 :`B` 1.0 :`A` 1.0) :`TextColorNormal` (struct :`R` 1.0 :`G` 1.0 :`B` 1.0 :`A` 1.0)) ; QUIT
)

(event `/Game/AnonsDialogSystem/Blueprints/BPI_DialogInterface.Dialog`
  (params (EventID :type Name) (SwitchID :type Integer) (DialogText :type Text))
  (`/Game/AnonsDialogSystem/Blueprints/BP_DialogSystem.GlobalDialogEvent` (`self.DialogSystem`) EventID)
  (switch `int` (`KismetStringLibrary.Conv_StringToInt` (`KismetStringLibrary.Conv_NameToString` EventID))
    (:`1`
      (`self.Gesture` "NewEnumerator15")
      (bind _dialogsystem (`/Game/AnonsDialogSystem/Blueprints/BP_DialogSystem.AddDialog` (stale `self.Talk` _dialogsystem) null "Guard" "The gate can only be opened from the opposite side." "None" (struct :`R` 1.0 :`G` 1.0 :`B` 1.0 :`A` 1.0) (struct :`G` 0.502887 :`B` 0.250158 :`A` 1.0) (struct :`R` 1.0 :`G` 1.0 :`B` 1.0 :`A` 1.0) "/Game/kosm_fps_assets/Misc/Fonts/rexlia_rg_Font.rexlia_rg_Font" null null 0.0 0.02 (`self.Dialogue SFX`) false true))
      (bind _dialogsystem_2 (`/Game/AnonsDialogSystem/Blueprints/BP_DialogSystem.AddResponse` :`self` _dialogsystem :`ResponseDialog` "What's behind it?" :`EventID` "2" :`ResponseFont` "/Game/kosm_fps_assets/Misc/Fonts/rexlia_rg_Font.rexlia_rg_Font" :`TextColorHovered` (struct :`G` 1.0 :`B` 0.502887 :`A` 1.0) :`TextColorNormal` (struct :`R` 1.0 :`G` 1.0 :`B` 1.0 :`A` 1.0)))
      (`/Game/AnonsDialogSystem/Blueprints/BP_DialogSystem.AddResponse` :`self` _dialogsystem_2 :`ResponseDialog` "I have to go now" :`EventID` "5" :`ResponseFont` "/Game/kosm_fps_assets/Misc/Fonts/rexlia_rg_Font.rexlia_rg_Font" :`TextColorHovered` (struct :`G` 0.715694 :`B` 1.0 :`A` 1.0) :`TextColorNormal` (struct :`R` 1.0 :`G` 1.0 :`B` 1.0 :`A` 1.0)) ; QUIT
    )
    (:`2`
      (`self.Gesture` "NewEnumerator16")
      (bind _dialogsystem_3 (`/Game/AnonsDialogSystem/Blueprints/BP_DialogSystem.AddDialog` (stale `self.Talk` _dialogsystem) null "Guard" "Our sacred structures, but lately it's become treacherous." "None" (struct :`R` 1.0 :`G` 1.0 :`B` 1.0 :`A` 1.0) (struct :`G` 0.502887 :`B` 0.250158 :`A` 1.0) (struct :`R` 1.0 :`G` 1.0 :`B` 1.0 :`A` 1.0) "/Game/kosm_fps_assets/Misc/Fonts/rexlia_rg_Font.rexlia_rg_Font" null null 0.0 0.02 (`self.Dialogue SFX`) false true))
      (bind _dialogsystem_4 (`/Game/AnonsDialogSystem/Blueprints/BP_DialogSystem.AddResponse` :`self` _dialogsystem_3 :`ResponseDialog` "Why?" :`EventID` "3" :`ResponseFont` "/Game/kosm_fps_assets/Misc/Fonts/rexlia_rg_Font.rexlia_rg_Font" :`TextColorHovered` (struct :`G` 1.0 :`B` 0.502887 :`A` 1.0) :`TextColorNormal` (struct :`R` 1.0 :`G` 1.0 :`B` 1.0 :`A` 1.0)))
      (`/Game/AnonsDialogSystem/Blueprints/BP_DialogSystem.AddResponse` :`self` _dialogsystem_4 :`ResponseDialog` "I have to go now" :`EventID` "5" :`ResponseFont` "/Game/kosm_fps_assets/Misc/Fonts/rexlia_rg_Font.rexlia_rg_Font" :`TextColorHovered` (struct :`G` 0.715694 :`B` 1.0 :`A` 1.0) :`TextColorNormal` (struct :`R` 1.0 :`G` 1.0 :`B` 1.0 :`A` 1.0)) ; QUIT
    )
    (:`3`
      (bind _dialogsystem_5 (`/Game/AnonsDialogSystem/Blueprints/BP_DialogSystem.AddDialog` (stale `self.Talk` _dialogsystem) null "Guard" "We don't know. All we know is that when we sent scouts, they kept dyin'." "None" (struct :`R` 1.0 :`G` 1.0 :`B` 1.0 :`A` 1.0) (struct :`G` 0.502887 :`B` 0.250158 :`A` 1.0) (struct :`R` 1.0 :`G` 1.0 :`B` 1.0 :`A` 1.0) "/Game/kosm_fps_assets/Misc/Fonts/rexlia_rg_Font.rexlia_rg_Font" null null 0.2 0.02 (`self.Dialogue SFX`) false true)) ; 3
      (`/Game/AnonsDialogSystem/Blueprints/BP_DialogSystem.AddResponse` :`self` _dialogsystem_5 :`ResponseDialog` "I have to go now" :`EventID` "5" :`ResponseFont` "/Game/kosm_fps_assets/Misc/Fonts/rexlia_rg_Font.rexlia_rg_Font" :`TextColorHovered` (struct :`G` 0.715694 :`B` 1.0 :`A` 1.0) :`TextColorNormal` (struct :`R` 1.0 :`G` 1.0 :`B` 1.0 :`A` 1.0)) ; QUIT
    )
    (:`4`
      (bind _dialogsystem_6 (`/Game/AnonsDialogSystem/Blueprints/BP_DialogSystem.AddDialog` (stale `self.Talk` _dialogsystem) null "Guard" "This cave connects to one of our outposts on the surface, you will find the Chief there." "None" (struct :`R` 1.0 :`G` 1.0 :`B` 1.0 :`A` 1.0) (struct :`G` 0.502887 :`B` 0.250158 :`A` 1.0) (struct :`R` 1.0 :`G` 1.0 :`B` 1.0 :`A` 1.0) "/Game/kosm_fps_assets/Misc/Fonts/rexlia_rg_Font.rexlia_rg_Font" null null 0.2 0.02 (`self.Dialogue SFX`) false true)) ; 4
      (bind _dialogsystem_7 (`/Game/AnonsDialogSystem/Blueprints/BP_DialogSystem.AddResponse` :`self` _dialogsystem_6 :`ResponseDialog` "[go back]" :`EventID` "1" :`ResponseFont` "/Game/kosm_fps_assets/Misc/Fonts/rexlia_rg_Font.rexlia_rg_Font" :`TextColorHovered` (struct :`G` 0.715694 :`B` 1.0 :`A` 1.0) :`TextColorNormal` (struct :`R` 1.0 :`G` 1.0 :`B` 1.0 :`A` 1.0)))
      (`/Game/AnonsDialogSystem/Blueprints/BP_DialogSystem.AddResponse` :`self` _dialogsystem_7 :`ResponseDialog` "I have to go now" :`EventID` "5" :`ResponseFont` "/Game/kosm_fps_assets/Misc/Fonts/rexlia_rg_Font.rexlia_rg_Font" :`TextColorHovered` (struct :`G` 0.715694 :`B` 1.0 :`A` 1.0) :`TextColorNormal` (struct :`R` 1.0 :`G` 1.0 :`B` 1.0 :`A` 1.0)) ; QUIT
    )
    (:`5`
      (`/Game/AnonsDialogSystem/Blueprints/BP_DialogSystem.AddDialog` (stale `self.Talk` _dialogsystem) null "Guard" "Sure." "quit" (struct :`R` 1.0 :`G` 1.0 :`B` 1.0 :`A` 1.0) (struct :`G` 0.502887 :`B` 0.250158 :`A` 1.0) (struct :`R` 1.0 :`G` 1.0 :`B` 1.0 :`A` 1.0) "/Game/kosm_fps_assets/Misc/Fonts/rexlia_rg_Font.rexlia_rg_Font" null null 0.2 0.02 (`self.Dialogue SFX`) false true) ; 5
    )))

(fn `UserConstructionScript`
  (`parent.UserConstructionScript`))