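; Keycard door for an Episode 2 mission that opens when the player character enters its trigger box carrying the matching keycard.
; A DoOnce-gated overlap checks the character's keycards, then calls OpenDoor and the Opened dispatcher, leaving the gate closed.
; OpenDoor plays sounds and a timeline that offsets the cube from its starting location.
; Without the key, it shows a "requires a key" widget with a locked sound, briefly debounced, and rearms the trigger.
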(event `Open Door`
  (bind _returnvalue (`SceneComponent.K2_GetComponentLocation` (`self.Cube`)))
  (`|ExecutionSequence`
    (:`then_0`
      (set `self.DoorStartLocation` _returnvalue))
    (:`then_1`
      (bind (_direction _newtrack_2) (`Timeline|DoorMovement`)
        (:`Update`
          (`self.SetTickableWhenPaused` true)
          (`SceneComponent.K2_SetWorldLocation` (`self.Cube`) (+ _newtrack_2 (`self.DoorStartLocation`)) false false))))
    (:`then_2`
      (`GameplayStatics.PlaySoundAtLocation` "/Game/MISSIONS/EP0/Audio/SC_TutorialDoor.SC_TutorialDoor" _returnvalue (struct) 1.0 1.0 0.0 null null null)
      (`GameplayStatics.PlaySound2D` "/Game/MISSIONS/EP2/Audio/SC_DoorUnlocked.SC_DoorUnlocked" 1.0 1.0 0.0 null null))))

(event `self.ReceiveBeginPlay`)

(event `self.Box.OnComponentBeginOverlap`
  (params (OverlappedComponent :type "PrimitiveComponent Object Reference") (OtherActor :type "Actor Object Reference") (OtherComp :type "PrimitiveComponent Object Reference") (OtherBodyIndex :type Integer) (bFromSweep :type Boolean) (SweepResult :type "HitResult Structure (by ref)"))
  (bind _asfps_movement_character_light_1_vq_3 (cast `/Game/Blueprints/CHARACTERS/fpsMovementCharacter_light_1_vq3` OtherActor))
  (`/Engine/EditorBlueprintResources/StandardMacros.DoOnce` false :!label _label
    (:`Completed`
      (if (`KismetArrayLibrary.Array_Contains` (`/Game/Blueprints/CHARACTERS/fpsMovementCharacter_light_1_vq3.Keycards` _asfps_movement_character_light_1_vq_3) (`self.Keycard Value`))
        (`self.Open Door`)
        (`self.opened`)
        (else
          (`|ExecutionSequence`
            (:`then_0`
              (`/Engine/EditorBlueprintResources/StandardMacros.DoOnce` false :!label _label_2
                (:`Completed`
                  (`/Game/Blueprints/NewFunctionLibrary.clean all message widgets`)
                  (`KismetSystemLibrary.Delay` 0.01)
                  (`GameplayStatics.PlaySound2D` "/Game/MISSIONS/EP2/Audio/SC_DoorLocked.SC_DoorLocked" 1.0 1.0 0.0 null null)
                  (bind _returnvalue (`|CreateWidget` "/Game/Blueprints/UI/UI_Pickups/UI_GenericMessage_alt.UI_GenericMessage_alt_C" null "this door requires a key"))
                  (`UserWidget.AddToViewport` _returnvalue 0)
                  (`KismetSystemLibrary.Delay` 0.2)
                  (goto _label_2 :!via `Reset`))))
            (:`then_1`
              (goto _label :!via `Reset`))))))))

(fn `UserConstructionScript`)