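; BP_EP2_Platform1 is a moving platform for EP2 that can crush the player, with a comment noting a fix for elevator clipping.
; After a starting delay, a timeline lerps the platform from its start to EndLocation at PlayRate, set to tick while paused.
; When CanCrush is set, a living player overlapping the Box triggers a DoOnce that kills them and stops the timeline.
; The player's respawn event re-arms the DoOnce.
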(event `self.ReceiveBeginPlay`
  (bind _player (`/Game/Blueprints/NewFunctionLibrary.get player`))
  (add `/Game/Blueprints/CHARACTERS/fpsMovementCharacter_light_1_vq3.respawned` _player (delegate `reset`))
  (`KismetSystemLibrary.Delay` (`self.Starting delay`))
  (set `self.PlatformStartLocation` (`SceneComponent.RelativeLocation` (`self.Platform`)))
  (set `self.PlatformEndLocation` (`SceneComponent.RelativeLocation` (`self.End_Location`)))
  (bind (_direction _newtrack_0) (`Timeline|DoorMovement` :!label _label)
    (:`Update`
      (`self.SetTickableWhenPaused` true)
      (`SceneComponent.K2_SetRelativeLocation` (`self.Platform`) (`KismetMathLibrary.VLerp` (`self.PlatformStartLocation`) (`self.PlatformEndLocation`) _newtrack_0) false false)
      (`TimelineComponent.SetPlayRate` (`self.DoorMovement`) (`self.Play rate`)))))

(event `reset`
  (goto _label_2 :!via `Reset`))

(event `stop`
  (goto _label :!via `Stop`))

(event `self.Box.OnComponentBeginOverlap`
  (params (OverlappedComponent :type "PrimitiveComponent Object Reference") (OtherActor :type "Actor Object Reference") (OtherComp :type "PrimitiveComponent Object Reference") (OtherBodyIndex :type Integer) (bFromSweep :type Boolean) (SweepResult :type "HitResult Structure (by ref)"))
  ;[1 1 1] solved the problem of elevator clipping through the player
  (bind _asfps_movement_character_light_1_vq_3 (cast `/Game/Blueprints/CHARACTERS/fpsMovementCharacter_light_1_vq3` OtherActor))
  (if (not (`/Game/Blueprints/CHARACTERS/fpsMovementCharacter_light_1_vq3.IsDead?` _asfps_movement_character_light_1_vq_3))
    (if (`self.Can crush?`)
      (`/Engine/EditorBlueprintResources/StandardMacros.DoOnce` false :!label _label_2
        (:`Completed`
          (`/Game/Blueprints/CHARACTERS/fpsMovementCharacter_light_1_vq3.IsDeadMulticast` _asfps_movement_character_light_1_vq_3)
          (`self.stop`))))))

(event `self.Box.OnComponentEndOverlap`
  (params (OverlappedComponent :type "PrimitiveComponent Object Reference") (OtherActor :type "Actor Object Reference") (OtherComp :type "PrimitiveComponent Object Reference") (OtherBodyIndex :type Integer)))

(event `self.Platform_collision.OnComponentHit`
  (params (HitComponent :type "PrimitiveComponent Object Reference") (OtherActor :type "Actor Object Reference") (OtherComp :type "PrimitiveComponent Object Reference") (NormalImpulse :type "Vector Structure") (Hit :type "HitResult Structure (by ref)")))

(fn `UserConstructionScript`)