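; Keycard pickup for an episode 2 mission that spins steadily and is collected when the player character overlaps its sphere.
; Pickup adds its keycard value to the player's Keycards, plays a sound and shows a pickup widget tinted with the card's color.
; It then calls PickedUp, destroys itself and decrements ItemsLeft if its parent actor is a BP_ItemCounter.
; A save-game branch is left unconnected.
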(event `self.Sphere.OnComponentBeginOverlap`
  (params (OverlappedComponent :type "PrimitiveComponent Object Reference") (OtherActor :type "Actor Object Reference") (OtherComp :type "PrimitiveComponent Object Reference") (OtherBodyIndex :type Integer) (bFromSweep :type Boolean) (SweepResult :type "HitResult Structure (by ref)"))
  (bind _asfps_movement_character_light_1_vq_3 (cast `/Game/Blueprints/CHARACTERS/fpsMovementCharacter_light_1_vq3` OtherActor))
  (`KismetArrayLibrary.Array_Add` (`/Game/Blueprints/CHARACTERS/fpsMovementCharacter_light_1_vq3.Keycards` _asfps_movement_character_light_1_vq_3) (`self.Keycard Value`))
  (`GameplayStatics.PlaySound2D` "/Game/AUDIO/SFX_Pickups/SC_KeyPickup.SC_KeyPickup" 1.0 1.0 0.0 null null)
  (bind _returnvalue (`|CreateWidget` "/Game/Blueprints/UI/UI_Pickups/UI_Pickup_Keycard.UI_Pickup_Keycard_C"))
  (set `/Game/Blueprints/UI/UI_Pickups/UI_Pickup_Keycard.Color` (`self.Keycard Color`) _returnvalue)
  (`UserWidget.AddToViewport` _returnvalue 0)
  (`|ExecutionSequence`
    (:`then_0`
      (`self.picked up`)
      (`self.K2_DestroyActor`))
    (:`then_1`
      (bind _asbp_item_counter (cast `/Game/Blueprints/MISC/BP_ItemCounter` (`self.GetParentActor`)))
      (bind _result (`/Engine/EditorBlueprintResources/StandardMacros.DecrementInt` (`/Game/Blueprints/MISC/BP_ItemCounter.Items left` _asbp_item_counter))
        (:`  `
          (set `/Game/Blueprints/MISC/BP_ItemCounter.Items left` _result _asbp_item_counter))))))

(event `self.Keycard.OnComponentBeginOverlap`
  (params (OverlappedComponent :type "PrimitiveComponent Object Reference") (OtherActor :type "Actor Object Reference") (OtherComp :type "PrimitiveComponent Object Reference") (OtherBodyIndex :type Integer) (bFromSweep :type Boolean) (SweepResult :type "HitResult Structure (by ref)")))

(event `self.ReceiveTick`
  (params (DeltaSeconds :type "Float (single-precision)"))
  ;[1 1 1] NEW ROTATION COMPONENT: FLOAT VALUE DEFINES ROTATION SPEED, ELIMINATED VETICAL FLOATING
  (`self.K2_AddActorLocalRotation` (`KismetMathLibrary.MakeRotator` 0.0 0.0 (* DeltaSeconds 45.0))))

(fn `UserConstructionScript`)