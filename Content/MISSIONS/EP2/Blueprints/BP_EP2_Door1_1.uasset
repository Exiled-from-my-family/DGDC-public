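; BP_EP2_Door1_1 is an automatic door for an Episode 2 mission that moves between its start and EndLocation when Characters use its trigger box.
; A timeline lerps the mesh after retriggerable delays that recheck overlaps, closing again unless Permanent is set.
; Sounds accompany movement, with AI noise events reported on opening and fully closing.
; Tick, switched on by trigger entry and off when movement finishes, flips direction if the player overlaps the moving door.
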(event `self.ReceiveBeginPlay`
  (set `self.DoorStartLocation` (`SceneComponent.RelativeLocation` (`self.Door`)))
  (set `self.DoorOpenLocation` (`SceneComponent.RelativeLocation` (`self.end_location`)))
  (`PrimitiveComponent.SetCollisionProfileName` (`self.Door`) "BlockAllDynamic" true))

(event `JUST OPEN IT`
  (bind _returnvalue (`SceneComponent.K2_GetComponentLocation` (`self.Door`)))
  (`|ExecutionSequence` :!label _label
    (:`then_0`
      (`/Engine/EditorBlueprintResources/StandardMacros.DoOnce` false :!label _label_2
        (:`Completed`
          (`GameplayStatics.PlaySoundAtLocation` (`self.Door SFX`) _returnvalue (struct) 0.75 (`self.Pitch`) 0.0 "/Game/kosm_fps_assets/Misc/SoundFX/SoundAttenuationNormal.SoundAttenuationNormal" null null)
          (`AISense_Hearing.ReportNoiseEvent` _returnvalue 1.0 null))))
    (:`then_1`
      (bind (_direction _float_track) (`Timeline|DoorMovement` :!label _label_3)
        (:`Update`
          (`self.SetTickableWhenPaused` true)
          (bind _sweephitresult (`SceneComponent.K2_SetRelativeLocation` (`self.Door`) (`KismetMathLibrary.VLerp` (`self.DoorStartLocation`) (`self.DoorOpenLocation`) _float_track) false false))
          (`TimelineComponent.SetPlayRate` (`self.DoorMovement`) (`self.Play rate`))
          (`KismetSystemLibrary.Delay` 0.2))
        (:`Finished`
          (switch `ETimelineDirection` _direction
            (:`Forward`
              (`self.SetActorTickEnabled` false))
            (:`Backward`
              (`GameplayStatics.PlaySoundAtLocation` (`self.Door_End`) _returnvalue (struct) 0.6 1.0 0.0 "/Game/kosm_fps_assets/Misc/SoundFX/SoundAttenuationLow.SoundAttenuationLow" null null)
              (`AISense_Hearing.ReportNoiseEvent` _returnvalue 1.0 null)
              (`self.SetActorTickEnabled` false)
              (goto _label_2 :!via `Reset`))))))))

(event `self.TriggerBox_Player.OnComponentBeginOverlap`
  (params (OverlappedComponent :type "PrimitiveComponent Object Reference") (OtherActor :type "Actor Object Reference") (OtherComp :type "PrimitiveComponent Object Reference") (OtherBodyIndex :type Integer) (bFromSweep :type Boolean) (SweepResult :type "HitResult Structure (by ref)"))
  (cast `Character` OtherActor)
  (`self.SetActorTickEnabled` true)
  (`KismetSystemLibrary.RetriggerableDelay` (`self.enter delay`))
  (if (`KismetMathLibrary.Conv_IntToBool` (`KismetArrayLibrary.Array_Length` (`PrimitiveComponent.GetOverlappingActors` (`self.TriggerBox_Player`) "/Script/Engine.Character")))
    (goto _label)))

(event `self.TriggerBox_Player.OnComponentEndOverlap`
  (params (OverlappedComponent :type "PrimitiveComponent Object Reference") (OtherActor :type "Actor Object Reference") (OtherComp :type "PrimitiveComponent Object Reference") (OtherBodyIndex :type Integer))
  (cast `Character` OtherActor)
  (if (not (`self.Permanent?`))
    (`KismetSystemLibrary.RetriggerableDelay` (`self.Delay`))
    (if (not (`KismetMathLibrary.Conv_IntToBool` (`KismetArrayLibrary.Array_Length` (`PrimitiveComponent.GetOverlappingActors` (`self.TriggerBox_Player`) "/Script/Engine.Character"))))
      (`|ExecutionSequence` :!label _label_4
        (:`then_0`
          (goto _label_3 :!via `Reverse`))
        (:`then_1`
          (`GameplayStatics.PlaySoundAtLocation` (`self.Door SFX`) (`SceneComponent.K2_GetComponentLocation` (`self.Door`)) (struct) 0.6 (`self.Pitch`) 0.0 "/Game/kosm_fps_assets/Misc/SoundFX/SoundAttenuationLow.SoundAttenuationLow" null null))))))

(event `self.ReceiveTick`
  (params (DeltaSeconds :type "Float (single-precision)"))
  (if (`PrimitiveComponent.IsOverlappingActor` (`self.Door`) (`/Game/Blueprints/NewFunctionLibrary.get player PURE`))
    (switch `ETimelineDirection` (stale `JUST OPEN IT` _direction)
      (:`Forward`
        (goto _label_4))
      (:`Backward`
        (goto _label)))))

(fn `UserConstructionScript`)