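; EP2 mission NPC blueprint for Flak Jack, running his branching conversation with the player.
; Talk builds the DialogSystem UI with a camera angle, greeting and responses, plays a gesture and sets the idle state.
; Dialog forwards each response's EventID globally, then switches on it for the next line, responses and, in some branches, gestures or camera moves.
; ID 9 says goodbye and changes the idle state; no response here leads to branches 3 or 5.
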(event `self.Talk`
  (`|ExecutionSequence`
    (:`then_0`
      (bind _dialogsystem (`/Game/AnonsDialogSystem/Blueprints/BP_DialogSystem.CreateDialogUI` :`self` (`self.DialogSystem`) :`GUITexture` "/Game/VN_UI/UI_Textures/T_Infolink_Dialogue_Flat.T_Infolink_Dialogue_Flat" :`MainSize` (1350.0 350.0) :`MainTranslation` (0.0 -25.0) :`MainBorderColor` (struct :`R` 0.300544 :`G` 0.752942 :`B` 0.491021 :`A` 1.0)))
      (bind _dialogsystem_2 (`/Game/AnonsDialogSystem/Blueprints/BP_DialogSystem.AddCameraAngle` _dialogsystem self 0.5 350.0 60.0 75.0 true)) ; Add center angle
      (`/Game/AnonsDialogSystem/Blueprints/BP_DialogSystem.AddDialog` _dialogsystem_2 null "Flak Jack" "Howdy, lil' lady." "None" (struct :`R` 1.0 :`G` 1.0 :`B` 1.0 :`A` 1.0) (struct :`G` 0.502887 :`B` 0.250158 :`A` 1.0) (struct :`R` 1.0 :`G` 1.0 :`B` 1.0 :`A` 1.0) "/Game/kosm_fps_assets/Misc/Fonts/rexlia_rg_Font.rexlia_rg_Font" null null 0.0 0.02 (`self.Dialogue SFX`) false true)
      (bind _dialogsystem_3 (`/Game/AnonsDialogSystem/Blueprints/BP_DialogSystem.AddDialog` _dialogsystem null "Flak Jack" "Howdy, lil' lady." "None" (struct :`R` 1.0 :`G` 1.0 :`B` 1.0 :`A` 1.0) (struct :`G` 0.502887 :`B` 0.250158 :`A` 1.0) (struct :`R` 1.0 :`G` 1.0 :`B` 1.0 :`A` 1.0) "/Game/kosm_fps_assets/Misc/Fonts/rexlia_rg_Font.rexlia_rg_Font" null null 0.0 0.02 (`self.Dialogue SFX`) false true))
      (bind _dialogsystem_4 (`/Game/AnonsDialogSystem/Blueprints/BP_DialogSystem.AddResponse` :`self` _dialogsystem_3 :`ResponseDialog` "Wow, you’re huge. And dead. And huge!" :`EventID` "1" :`ResponseFont` "/Game/kosm_fps_assets/Misc/Fonts/rexlia_rg_Font.rexlia_rg_Font" :`TextColorHovered` (struct :`G` 1.0 :`B` 0.502887 :`A` 1.0) :`TextColorNormal` (struct :`R` 1.0 :`G` 1.0 :`B` 1.0 :`A` 1.0)))
      (bind _dialogsystem_5 (`/Game/AnonsDialogSystem/Blueprints/BP_DialogSystem.AddResponse` :`self` _dialogsystem_4 :`ResponseDialog` "Can you tell me more about the others?" :`EventID` "2" :`ResponseFont` "/Game/kosm_fps_assets/Misc/Fonts/rexlia_rg_Font.rexlia_rg_Font" :`TextColorHovered` (struct :`G` 1.0 :`B` 0.502887 :`A` 1.0) :`TextColorNormal` (struct :`R` 1.0 :`G` 1.0 :`B` 1.0 :`A` 1.0)))
      (`/Game/AnonsDialogSystem/Blueprints/BP_DialogSystem.AddResponse` :`self` _dialogsystem_5 :`ResponseDialog` "I have to go now" :`EventID` "9" :`ResponseFont` "/Game/kosm_fps_assets/Misc/Fonts/rexlia_rg_Font.rexlia_rg_Font" :`TextColorHovered` (struct :`G` 0.715694 :`B` 1.0 :`A` 1.0) :`TextColorNormal` (struct :`R` 1.0 :`G` 1.0 :`B` 1.0 :`A` 1.0)) ; QUIT
    )
    (:`then_1`
      (`self.Gesture` "NewEnumerator15"))
    (:`then_2`
      (set `self.Idle_Enum` "NewEnumerator0"))))

(event `/Game/AnonsDialogSystem/Blueprints/BPI_DialogInterface.Dialog`
  (params (EventID :type Name) (SwitchID :type Integer) (DialogText :type Text))
  (`/Game/AnonsDialogSystem/Blueprints/BP_DialogSystem.GlobalDialogEvent` (`self.DialogSystem`) EventID)
  (switch `int` (`KismetStringLibrary.Conv_StringToInt` (`KismetStringLibrary.Conv_NameToString` EventID))
    (:`1`
      (`self.Gesture` "NewEnumerator15")
      (bind _dialogsystem (`/Game/AnonsDialogSystem/Blueprints/BP_DialogSystem.AddCameraAngle` (stale `self.Talk` _dialogsystem) self 1.0 350.0 70.0 40.0 true)) ; 1
      (bind _dialogsystem_2 (`/Game/AnonsDialogSystem/Blueprints/BP_DialogSystem.AddDialog` _dialogsystem null "Flak Jack" "Yeah, I am a friggin’ hulk covered in plates. Could’ve been dealt a worse hand." "None" (struct :`R` 1.0 :`G` 1.0 :`B` 1.0 :`A` 1.0) (struct :`G` 0.502887 :`B` 0.250158 :`A` 1.0) (struct :`R` 1.0 :`G` 1.0 :`B` 1.0 :`A` 1.0) "/Game/kosm_fps_assets/Misc/Fonts/rexlia_rg_Font.rexlia_rg_Font" null null 0.0 0.02 (`self.Dialogue SFX`) false true))
      (bind _dialogsystem_3 (`/Game/AnonsDialogSystem/Blueprints/BP_DialogSystem.AddResponse` :`self` _dialogsystem_2 :`ResponseDialog` "Oh. And what about your past life?" :`EventID` "4" :`ResponseFont` "/Game/kosm_fps_assets/Misc/Fonts/rexlia_rg_Font.rexlia_rg_Font" :`TextColorHovered` (struct :`G` 1.0 :`B` 0.502887 :`A` 1.0) :`TextColorNormal` (struct :`R` 1.0 :`G` 1.0 :`B` 1.0 :`A` 1.0)))
      (bind _dialogsystem_4 (`/Game/AnonsDialogSystem/Blueprints/BP_DialogSystem.AddResponse` :`self` _dialogsystem_3 :`ResponseDialog` "What can you tell me about \"interferences\"? " :`EventID` "6" :`ResponseFont` "/Game/kosm_fps_assets/Misc/Fonts/rexlia_rg_Font.rexlia_rg_Font" :`TextColorHovered` (struct :`G` 1.0 :`B` 0.502887 :`A` 1.0) :`TextColorNormal` (struct :`R` 1.0 :`G` 1.0 :`B` 1.0 :`A` 1.0)))
      (`/Game/AnonsDialogSystem/Blueprints/BP_DialogSystem.AddResponse` :`self` _dialogsystem_4 :`ResponseDialog` "I have to go now" :`EventID` "9" :`ResponseFont` "/Game/kosm_fps_assets/Misc/Fonts/rexlia_rg_Font.rexlia_rg_Font" :`TextColorHovered` (struct :`G` 0.715694 :`B` 1.0 :`A` 1.0) :`TextColorNormal` (struct :`R` 1.0 :`G` 1.0 :`B` 1.0 :`A` 1.0)) ; QUIT
    )
    (:`2`
      (`self.Gesture` "NewEnumerator16")
      (bind _dialogsystem_5 (`/Game/AnonsDialogSystem/Blueprints/BP_DialogSystem.AddCameraAngle` (stale `self.Talk` _dialogsystem) self 1.2 400.0 60.0 -40.0 true)) ; 2
      (bind _dialogsystem_6 (`/Game/AnonsDialogSystem/Blueprints/BP_DialogSystem.AddDialog` _dialogsystem_5 null "Flak Jack" "I’ll keep it short. Major is major cuckoo. Wendy – more brawn than brains, Helsing is moping around and the robot is just unhinged." "None" (struct :`R` 1.0 :`G` 1.0 :`B` 1.0 :`A` 1.0) (struct :`G` 0.502887 :`B` 0.250158 :`A` 1.0) (struct :`R` 1.0 :`G` 1.0 :`B` 1.0 :`A` 1.0) "/Game/kosm_fps_assets/Misc/Fonts/rexlia_rg_Font.rexlia_rg_Font" null null 0.0 0.02 (`self.Dialogue SFX`) false true))
      (bind _dialogsystem_7 (`/Game/AnonsDialogSystem/Blueprints/BP_DialogSystem.AddResponse` :`self` _dialogsystem_6 :`ResponseDialog` "Teaming up with Rumble dude has been an experience" :`EventID` "8" :`ResponseFont` "/Game/kosm_fps_assets/Misc/Fonts/rexlia_rg_Font.rexlia_rg_Font" :`TextColorHovered` (struct :`G` 1.0 :`B` 0.502887 :`A` 1.0) :`TextColorNormal` (struct :`R` 1.0 :`G` 1.0 :`B` 1.0 :`A` 1.0)))
      (bind _dialogsystem_8 (`/Game/AnonsDialogSystem/Blueprints/BP_DialogSystem.AddResponse` :`self` _dialogsystem_7 :`ResponseDialog` "[go back]" :`EventID` "1" :`ResponseFont` "/Game/kosm_fps_assets/Misc/Fonts/rexlia_rg_Font.rexlia_rg_Font" :`TextColorHovered` (struct :`G` 0.715694 :`B` 1.0 :`A` 1.0) :`TextColorNormal` (struct :`R` 1.0 :`G` 1.0 :`B` 1.0 :`A` 1.0)))
      (`/Game/AnonsDialogSystem/Blueprints/BP_DialogSystem.AddResponse` :`self` _dialogsystem_8 :`ResponseDialog` "I have to go now" :`EventID` "9" :`ResponseFont` "/Game/kosm_fps_assets/Misc/Fonts/rexlia_rg_Font.rexlia_rg_Font" :`TextColorHovered` (struct :`G` 0.715694 :`B` 1.0 :`A` 1.0) :`TextColorNormal` (struct :`R` 1.0 :`G` 1.0 :`B` 1.0 :`A` 1.0)) ; QUIT
    )
    (:`3`
      (`self.Gesture` "NewEnumerator15")
      (bind _dialogsystem_9 (`/Game/AnonsDialogSystem/Blueprints/BP_DialogSystem.AddCameraAngle` (stale `self.Talk` _dialogsystem) (`GameplayStatics.GetPlayerCharacter` 0) 1.0 350.0 70.0 -40.0 true)) ; 3
      (bind _dialogsystem_10 (`/Game/AnonsDialogSystem/Blueprints/BP_DialogSystem.AddDialog` _dialogsystem_9 null "Flak Jack" "Well, I liked to eat, got plenty of exercise and carried a concealed .45 for safety. You know, a normal, quiet life. No surprises." "None" (struct :`R` 1.0 :`G` 1.0 :`B` 1.0 :`A` 1.0) (struct :`G` 0.502887 :`B` 0.250158 :`A` 1.0) (struct :`R` 1.0 :`G` 1.0 :`B` 1.0 :`A` 1.0) "/Game/kosm_fps_assets/Misc/Fonts/rexlia_rg_Font.rexlia_rg_Font" null null 0.0 0.02 (`self.Dialogue SFX`) false true))
      (bind _dialogsystem_11 (`/Game/AnonsDialogSystem/Blueprints/BP_DialogSystem.AddResponse` :`self` _dialogsystem_10 :`ResponseDialog` "What’s your last memory?" :`EventID` "4" :`ResponseFont` "/Game/kosm_fps_assets/Misc/Fonts/rexlia_rg_Font.rexlia_rg_Font" :`TextColorHovered` (struct :`G` 1.0 :`B` 0.502887 :`A` 1.0) :`TextColorNormal` (struct :`R` 1.0 :`G` 1.0 :`B` 1.0 :`A` 1.0)))
      (bind _dialogsystem_12 (`/Game/AnonsDialogSystem/Blueprints/BP_DialogSystem.AddResponse` :`self` _dialogsystem_11 :`ResponseDialog` "What can you tell me about \"interferences\"? " :`EventID` "6" :`ResponseFont` "/Game/kosm_fps_assets/Misc/Fonts/rexlia_rg_Font.rexlia_rg_Font" :`TextColorHovered` (struct :`G` 1.0 :`B` 0.502887 :`A` 1.0) :`TextColorNormal` (struct :`R` 1.0 :`G` 1.0 :`B` 1.0 :`A` 1.0)))
      (`/Game/AnonsDialogSystem/Blueprints/BP_DialogSystem.AddResponse` :`self` _dialogsystem_12 :`ResponseDialog` "I have to go now" :`EventID` "9" :`ResponseFont` "/Game/kosm_fps_assets/Misc/Fonts/rexlia_rg_Font.rexlia_rg_Font" :`TextColorHovered` (struct :`G` 0.715694 :`B` 1.0 :`A` 1.0) :`TextColorNormal` (struct :`R` 1.0 :`G` 1.0 :`B` 1.0 :`A` 1.0)) ; QUIT
    )
    (:`4`
      (bind _dialogsystem_13 (`/Game/AnonsDialogSystem/Blueprints/BP_DialogSystem.AddCameraAngle` (stale `self.Talk` _dialogsystem) self 1.0 350.0 70.0 -40.0 true)) ; 4
      (bind _dialogsystem_14 (`/Game/AnonsDialogSystem/Blueprints/BP_DialogSystem.AddDialog` _dialogsystem_13 null "Flak Jack" "I was mixin’ fertilizer and bam! Now I’m this… thing." "None" (struct :`R` 1.0 :`G` 1.0 :`B` 1.0 :`A` 1.0) (struct :`G` 0.502887 :`B` 0.250158 :`A` 1.0) (struct :`R` 1.0 :`G` 1.0 :`B` 1.0 :`A` 1.0) "/Game/kosm_fps_assets/Misc/Fonts/rexlia_rg_Font.rexlia_rg_Font" null null 0.0 0.02 (`self.Dialogue SFX`) false true))
      (bind _dialogsystem_15 (`/Game/AnonsDialogSystem/Blueprints/BP_DialogSystem.AddResponse` :`self` _dialogsystem_14 :`ResponseDialog` "What can you tell me about \"interferences\"? " :`EventID` "6" :`ResponseFont` "/Game/kosm_fps_assets/Misc/Fonts/rexlia_rg_Font.rexlia_rg_Font" :`TextColorHovered` (struct :`G` 1.0 :`B` 0.502887 :`A` 1.0) :`TextColorNormal` (struct :`R` 1.0 :`G` 1.0 :`B` 1.0 :`A` 1.0)))
      (bind _dialogsystem_16 (`/Game/AnonsDialogSystem/Blueprints/BP_DialogSystem.AddResponse` :`self` _dialogsystem_15 :`ResponseDialog` "[go back]" :`EventID` "1" :`ResponseFont` "/Game/kosm_fps_assets/Misc/Fonts/rexlia_rg_Font.rexlia_rg_Font" :`TextColorHovered` (struct :`G` 0.715694 :`B` 1.0 :`A` 1.0) :`TextColorNormal` (struct :`R` 1.0 :`G` 1.0 :`B` 1.0 :`A` 1.0)))
      (`/Game/AnonsDialogSystem/Blueprints/BP_DialogSystem.AddResponse` :`self` _dialogsystem_16 :`ResponseDialog` "I have to go now" :`EventID` "9" :`ResponseFont` "/Game/kosm_fps_assets/Misc/Fonts/rexlia_rg_Font.rexlia_rg_Font" :`TextColorHovered` (struct :`G` 0.715694 :`B` 1.0 :`A` 1.0) :`TextColorNormal` (struct :`R` 1.0 :`G` 1.0 :`B` 1.0 :`A` 1.0)) ; QUIT
    )
    (:`5`
      (`self.Gesture` "NewEnumerator16")
      (bind _dialogsystem_17 (`/Game/AnonsDialogSystem/Blueprints/BP_DialogSystem.AddDialog` (stale `self.Talk` _dialogsystem) null "Flak Jack" "Well I’ll be damned - I was minding my own business mixin’ fertilizer, next thing I know I wake up as an army beefcake. Ah, whatever…" "None" (struct :`R` 1.0 :`G` 1.0 :`B` 1.0 :`A` 1.0) (struct :`G` 0.502887 :`B` 0.250158 :`A` 1.0) (struct :`R` 1.0 :`G` 1.0 :`B` 1.0 :`A` 1.0) "/Game/kosm_fps_assets/Misc/Fonts/rexlia_rg_Font.rexlia_rg_Font" null null 0.0 0.02 (`self.Dialogue SFX`) false true))
      (bind _dialogsystem_18 (`/Game/AnonsDialogSystem/Blueprints/BP_DialogSystem.AddResponse` :`self` _dialogsystem_17 :`ResponseDialog` "What can you tell me about \"interferences\"? " :`EventID` "6" :`ResponseFont` "/Game/kosm_fps_assets/Misc/Fonts/rexlia_rg_Font.rexlia_rg_Font" :`TextColorHovered` (struct :`G` 1.0 :`B` 0.502887 :`A` 1.0) :`TextColorNormal` (struct :`R` 1.0 :`G` 1.0 :`B` 1.0 :`A` 1.0)))
      (bind _dialogsystem_19 (`/Game/AnonsDialogSystem/Blueprints/BP_DialogSystem.AddResponse` :`self` _dialogsystem_18 :`ResponseDialog` "[go back]" :`EventID` "1" :`ResponseFont` "/Game/kosm_fps_assets/Misc/Fonts/rexlia_rg_Font.rexlia_rg_Font" :`TextColorHovered` (struct :`G` 0.715694 :`B` 1.0 :`A` 1.0) :`TextColorNormal` (struct :`R` 1.0 :`G` 1.0 :`B` 1.0 :`A` 1.0)))
      (`/Game/AnonsDialogSystem/Blueprints/BP_DialogSystem.AddResponse` :`self` _dialogsystem_19 :`ResponseDialog` "I have to go now" :`EventID` "9" :`ResponseFont` "/Game/kosm_fps_assets/Misc/Fonts/rexlia_rg_Font.rexlia_rg_Font" :`TextColorHovered` (struct :`G` 0.715694 :`B` 1.0 :`A` 1.0) :`TextColorNormal` (struct :`R` 1.0 :`G` 1.0 :`B` 1.0 :`A` 1.0)) ; QUIT
    )
    (:`6`
      (`self.Gesture` "NewEnumerator15")
      (`/Game/AnonsDialogSystem/Blueprints/BP_DialogSystem.AddCameraAngle` (stale `self.Talk` _dialogsystem) self 1.5 500.0 75.0 -60.0 true) ; 6
      (bind _dialogsystem_20 (`/Game/AnonsDialogSystem/Blueprints/BP_DialogSystem.AddDialog` (stale `self.Talk` _dialogsystem) null "Flak Jack" "Yeah… We got a weird guest visit every time a new soul was summoned." "None" (struct :`R` 1.0 :`G` 1.0 :`B` 1.0 :`A` 1.0) (struct :`G` 0.502887 :`B` 0.250158 :`A` 1.0) (struct :`R` 1.0 :`G` 1.0 :`B` 1.0 :`A` 1.0) "/Game/kosm_fps_assets/Misc/Fonts/rexlia_rg_Font.rexlia_rg_Font" null null 0.0 0.02 (`self.Dialogue SFX`) false true)) ; 6
      (bind _dialogsystem_21 (`/Game/AnonsDialogSystem/Blueprints/BP_DialogSystem.AddResponse` :`self` _dialogsystem_20 :`ResponseDialog` "And I am the last one to join..." :`EventID` "7" :`ResponseFont` "/Game/kosm_fps_assets/Misc/Fonts/rexlia_rg_Font.rexlia_rg_Font" :`TextColorHovered` (struct :`G` 1.0 :`B` 0.502887 :`A` 1.0) :`TextColorNormal` (struct :`R` 1.0 :`G` 1.0 :`B` 1.0 :`A` 1.0)))
      (bind _dialogsystem_22 (`/Game/AnonsDialogSystem/Blueprints/BP_DialogSystem.AddResponse` :`self` _dialogsystem_21 :`ResponseDialog` "[go back]" :`EventID` "1" :`ResponseFont` "/Game/kosm_fps_assets/Misc/Fonts/rexlia_rg_Font.rexlia_rg_Font" :`TextColorHovered` (struct :`G` 0.715694 :`B` 1.0 :`A` 1.0) :`TextColorNormal` (struct :`R` 1.0 :`G` 1.0 :`B` 1.0 :`A` 1.0)))
      (`/Game/AnonsDialogSystem/Blueprints/BP_DialogSystem.AddResponse` :`self` _dialogsystem_22 :`ResponseDialog` "I have to go now" :`EventID` "9" :`ResponseFont` "/Game/kosm_fps_assets/Misc/Fonts/rexlia_rg_Font.rexlia_rg_Font" :`TextColorHovered` (struct :`G` 0.715694 :`B` 1.0 :`A` 1.0) :`TextColorNormal` (struct :`R` 1.0 :`G` 1.0 :`B` 1.0 :`A` 1.0)) ; QUIT
    )
    (:`7`
      (`self.Gesture` "NewEnumerator16")
      (bind _dialogsystem_23 (`/Game/AnonsDialogSystem/Blueprints/BP_DialogSystem.AddDialog` (stale `self.Talk` _dialogsystem) null "Flak Jack" "Indeed. Keep your guard up, lil' lady." "None" (struct :`R` 1.0 :`G` 1.0 :`B` 1.0 :`A` 1.0) (struct :`G` 0.502887 :`B` 0.250158 :`A` 1.0) (struct :`R` 1.0 :`G` 1.0 :`B` 1.0 :`A` 1.0) "/Game/kosm_fps_assets/Misc/Fonts/rexlia_rg_Font.rexlia_rg_Font" null null 0.0 0.02 (`self.Dialogue SFX`) false true))
      (bind _dialogsystem_24 (`/Game/AnonsDialogSystem/Blueprints/BP_DialogSystem.AddResponse` :`self` _dialogsystem_23 :`ResponseDialog` "[go back]" :`EventID` "1" :`ResponseFont` "/Game/kosm_fps_assets/Misc/Fonts/rexlia_rg_Font.rexlia_rg_Font" :`TextColorHovered` (struct :`G` 0.715694 :`B` 1.0 :`A` 1.0) :`TextColorNormal` (struct :`R` 1.0 :`G` 1.0 :`B` 1.0 :`A` 1.0)))
      (`/Game/AnonsDialogSystem/Blueprints/BP_DialogSystem.AddResponse` :`self` _dialogsystem_24 :`ResponseDialog` "I have to go now" :`EventID` "9" :`ResponseFont` "/Game/kosm_fps_assets/Misc/Fonts/rexlia_rg_Font.rexlia_rg_Font" :`TextColorHovered` (struct :`G` 0.715694 :`B` 1.0 :`A` 1.0) :`TextColorNormal` (struct :`R` 1.0 :`G` 1.0 :`B` 1.0 :`A` 1.0)) ; QUIT
    )
    (:`8`
      (`self.Gesture` "NewEnumerator16")
      (bind _dialogsystem_25 (`/Game/AnonsDialogSystem/Blueprints/BP_DialogSystem.AddDialog` (stale `self.Talk` _dialogsystem) null "Flak Jack" "Yes, he tends to fill the comms with his ramblings, but he’s not as dumb as it seems. You should check on him, he’s your team." "None" (struct :`R` 1.0 :`G` 1.0 :`B` 1.0 :`A` 1.0) (struct :`G` 0.502887 :`B` 0.250158 :`A` 1.0) (struct :`R` 1.0 :`G` 1.0 :`B` 1.0 :`A` 1.0) "/Game/kosm_fps_assets/Misc/Fonts/rexlia_rg_Font.rexlia_rg_Font" null null 0.0 0.02 (`self.Dialogue SFX`) false true)) ; 8
      (bind _dialogsystem_26 (`/Game/AnonsDialogSystem/Blueprints/BP_DialogSystem.AddResponse` :`self` _dialogsystem_25 :`ResponseDialog` "[go back]" :`EventID` "1" :`ResponseFont` "/Game/kosm_fps_assets/Misc/Fonts/rexlia_rg_Font.rexlia_rg_Font" :`TextColorHovered` (struct :`G` 0.715694 :`B` 1.0 :`A` 1.0) :`TextColorNormal` (struct :`R` 1.0 :`G` 1.0 :`B` 1.0 :`A` 1.0)))
      (`/Game/AnonsDialogSystem/Blueprints/BP_DialogSystem.AddResponse` :`self` _dialogsystem_26 :`ResponseDialog` "I have to go now" :`EventID` "9" :`ResponseFont` "/Game/kosm_fps_assets/Misc/Fonts/rexlia_rg_Font.rexlia_rg_Font" :`TextColorHovered` (struct :`G` 0.715694 :`B` 1.0 :`A` 1.0) :`TextColorNormal` (struct :`R` 1.0 :`G` 1.0 :`B` 1.0 :`A` 1.0)) ; QUIT
    )
    (:`9`
      (`/Game/AnonsDialogSystem/Blueprints/BP_DialogSystem.AddDialog` (stale `self.Talk` _dialogsystem) null "Flak Jack" "See you around." "quit" (struct :`R` 1.0 :`G` 1.0 :`B` 1.0 :`A` 1.0) (struct :`G` 0.502887 :`B` 0.250158 :`A` 1.0) (struct :`R` 1.0 :`G` 1.0 :`B` 1.0 :`A` 1.0) "/Game/kosm_fps_assets/Misc/Fonts/rexlia_rg_Font.rexlia_rg_Font" null null 0.2 0.02 (`self.Dialogue SFX`) false true) ; 9
      (set `self.Idle_Enum` "NewEnumerator1"))))

(fn `UserConstructionScript`
  (`parent.UserConstructionScript`))