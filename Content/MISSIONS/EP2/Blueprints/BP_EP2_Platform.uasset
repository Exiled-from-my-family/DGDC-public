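; BP_EP2_Platform is a moving platform actor for Episode 2 missions.
; After a configurable starting delay on BeginPlay, it records the platform's world location and plays the DoorMovement timeline.
; Each update offsets the platform by the timeline's vector track, applies a configurable play rate, and sets the actor tickable when paused.
; Leftover reverse and replay logic is never executed.
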(event `self.ReceiveBeginPlay`
  (`KismetSystemLibrary.Delay` (`self.Starting delay`))
  (set `self.DoorStartLocation` (`SceneComponent.K2_GetComponentLocation` (`self.Platform`)))
  (bind (_direction _newtrack_2) (`Timeline|DoorMovement`)
    (:`Update`
      (`self.SetTickableWhenPaused` true)
      (`SceneComponent.K2_SetWorldLocation` (`self.Platform`) (+ _newtrack_2 (`self.DoorStartLocation`)) false false)
      (`TimelineComponent.SetPlayRate` (`self.DoorMovement`) (`self.Play rate`)))))

(fn `UserConstructionScript`)