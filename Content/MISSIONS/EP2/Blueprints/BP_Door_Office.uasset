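; Office door for Episode 2 that swings open once, the first time the player's FPS character enters its trigger box.
; OpenDoor plays a metal door sound and runs a timeline that lerps the door's relative rotation, with collision disabled until the swing finishes.
; A keycard check with a locked-door sound and timed message widget remains in the graph but is disconnected, so the door needs no key.
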(event `Open Door`
  (`|ExecutionSequence`
    (:`then_0`
      (`PrimitiveComponent.SetCollisionEnabled` (`self.Door`) "NoCollision")
      (bind (_direction _rotate) (`Timeline|DoorMovement` :!via `PlayFromStart`)
        (:`Update`
          (`self.SetTickableWhenPaused` true)
          (`SceneComponent.K2_SetRelativeRotation` (`self.Door`) (`KismetMathLibrary.RLerp` (struct :`Yaw` 90.0) (`self.Rotation`) _rotate) false false))
        (:`Finished`
          (`PrimitiveComponent.SetCollisionEnabled` (`self.Door`) "QueryAndPhysics"))))
    (:`then_1`
      (`GameplayStatics.PlaySoundAtLocation` "/Game/AUDIO/SFX_Doors/SW_DoorMetal_Open.SW_DoorMetal_Open" (`SceneComponent.K2_GetComponentLocation` (`self.Door`)) (struct) 1.0 1.0 0.0 "/Game/kosm_fps_assets/Misc/SoundFX/SoundAttenuationLow.SoundAttenuationLow" null null))))

(event `self.ReceiveBeginPlay`)

(event `self.Box.OnComponentBeginOverlap`
  (params (OverlappedComponent :type "PrimitiveComponent Object Reference") (OtherActor :type "Actor Object Reference") (OtherComp :type "PrimitiveComponent Object Reference") (OtherBodyIndex :type Integer) (bFromSweep :type Boolean) (SweepResult :type "HitResult Structure (by ref)"))
  (bind _asfps_movement_character_light_1_vq_3 (cast `/Game/Blueprints/CHARACTERS/fpsMovementCharacter_light_1_vq3` OtherActor))
  (`/Engine/EditorBlueprintResources/StandardMacros.DoOnce` false
    (:`Completed`
      (`self.Open Door`))))

(fn `UserConstructionScript`)