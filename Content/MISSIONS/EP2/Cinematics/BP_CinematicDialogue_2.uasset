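; Cinematic dialogue Blueprint for Episode 2, holding character lines for the Dominance intro, match outcomes, misfired-portal scene and Hacker encounter.
; Dialogue maps a line number to a hard-coded portrait, speaker and text, shown in a new skippable infolink cutscene widget.
; Quit restores the player HUD and removes infolink widgets.
; Bossend fades to black with audio, shows a loading screen and opens the EP2 hub level.
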(event `Boss end`
  (`PlayerCameraManager.StartCameraFade` (`GameplayStatics.GetPlayerCameraManager` 0) 0.0 1.0 2.0 (struct :`A` 1.0) true true)
  (`KismetSystemLibrary.Delay` 2.0)
  (bind _returnvalue (`|CreateWidget` "/Game/Blueprints/UI/UI_LoadingScreen.UI_LoadingScreen_C"))
  (`UserWidget.AddToViewport` _returnvalue 0)
  (`KismetSystemLibrary.Delay` 1.0)
  (`GameplayStatics.OpenLevel` "EP2_HUB_ml"))

(event `Quit`
  (bind _player (`/Game/Blueprints/NewFunctionLibrary.get player`))
  (`Widget.SetVisibility` (`/Game/Blueprints/CHARACTERS/fpsMovementCharacter_light_1_vq3.HUD` _player) "Visible")
  (bind _foundwidgets (`WidgetBlueprintLibrary.GetAllWidgetsOfClass` "/Game/VN_UI/BP_infolink_cutscene.BP_infolink_cutscene_C"))
  (`Widget.RemoveFromParent` _foundwidgets))

(event `Dialogue`
  (params (Line :type Integer :default 1))
  (switch `int` Line
    (:`1`
      ;[1 1 1] DOM1
      (bind _returnvalue (`|CreateWidget` "/Game/VN_UI/BP_infolink_cutscene.BP_infolink_cutscene_C"))
      (`UserWidget.AddToViewport` _returnvalue 0)
      (`/Game/VN_UI/BP_infolink_cutscene.MESSAGE` _returnvalue "/Game/VN_UI/Avatars/T_Infolink_MajorCommando.T_Infolink_MajorCommando" "Hey, everyone! We’ve got a new pal!" "Major "))
    (:`2`
      (bind _returnvalue_2 (`|CreateWidget` "/Game/VN_UI/BP_infolink_cutscene.BP_infolink_cutscene_C"))
      (`UserWidget.AddToViewport` _returnvalue_2 0)
      (`/Game/VN_UI/BP_infolink_cutscene.MESSAGE` _returnvalue_2 "/Game/VN_UI/Avatars/T_Infolink_FlakJack.T_Infolink_FlakJack" "Welcome to the nuthouse, lil’ lady." "Flak Jack"))
    (:`3`
      (bind _returnvalue_3 (`|CreateWidget` "/Game/VN_UI/BP_infolink_cutscene.BP_infolink_cutscene_C"))
      (`UserWidget.AddToViewport` _returnvalue_3 0)
      (`/Game/VN_UI/BP_infolink_cutscene.MESSAGE` _returnvalue_3 "/Game/VN_UI/Avatars/T_Infolink_Wendy.T_Infolink_Wendy" "Oh, finally! I thought I was going to be the sole lady in this game, phew!" "Wendy"))
    (:`4`
      (bind _returnvalue_4 (`|CreateWidget` "/Game/VN_UI/BP_infolink_cutscene.BP_infolink_cutscene_C"))
      (`UserWidget.AddToViewport` _returnvalue_4 0)
      (`/Game/VN_UI/BP_infolink_cutscene.MESSAGE` _returnvalue_4 "/Game/VN_UI/Avatars/T_Infolink_MajorCommando.T_Infolink_MajorCommando" "Molly, look, we have a robot as well. Hey, robot, say hi to the new girl!" "Major"))
    (:`5`
      (bind _returnvalue_5 (`|CreateWidget` "/Game/VN_UI/BP_infolink_cutscene.BP_infolink_cutscene_C"))
      (`UserWidget.AddToViewport` _returnvalue_5 0)
      (`/Game/VN_UI/BP_infolink_cutscene.MESSAGE` _returnvalue_5 "/Game/VN_UI/Avatars/T_Infolink_Rumbletron.T_Infolink_Rumbletron" "..." "Rumbletron"))
    (:`6`
      (bind _returnvalue_6 (`|CreateWidget` "/Game/VN_UI/BP_infolink_cutscene.BP_infolink_cutscene_C"))
      (`UserWidget.AddToViewport` _returnvalue_6 0)
      (`/Game/VN_UI/BP_infolink_cutscene.MESSAGE` _returnvalue_6 "/Game/VN_UI/Avatars/T_Infolink_MajorCommando.T_Infolink_MajorCommando" "Ah, still out cold?" "Major"))
    (:`7`
      (bind _returnvalue_7 (`|CreateWidget` "/Game/VN_UI/BP_infolink_cutscene.BP_infolink_cutscene_C"))
      (`UserWidget.AddToViewport` _returnvalue_7 0)
      (`/Game/VN_UI/BP_infolink_cutscene.MESSAGE` _returnvalue_7 "/Game/VN_UI/Avatars/T_Infolink_Helsing.T_Infolink_Helsing" "Greetings. I am an occult hunter. You can call me Helsing I suppose, since this shabby ritual made me forget my past." "Helsing"))
    (:`8`
      (bind _returnvalue_8 (`|CreateWidget` "/Game/VN_UI/BP_infolink_cutscene.BP_infolink_cutscene_C"))
      (`UserWidget.AddToViewport` _returnvalue_8 0)
      (`/Game/VN_UI/BP_infolink_cutscene.MESSAGE` _returnvalue_8 "/Game/VN_UI/Avatars/T_Infolink_Wizard.T_Infolink_Wizard" "Ok, that will be enough. Now – a new mode of combat! \nTime to conquer Dominance Zones!" "Wizard"))
    (:`9`
      (bind _returnvalue_9 (`|CreateWidget` "/Game/VN_UI/BP_infolink_cutscene.BP_infolink_cutscene_C"))
      (`UserWidget.AddToViewport` _returnvalue_9 0)
      (`/Game/VN_UI/BP_infolink_cutscene.MESSAGE` _returnvalue_9 "/Game/VN_UI/Avatars/T_Infolink_Molly.T_Infolink_Molly" "Oh, like in the King of the-" "Molly"))
    (:`10`
      (bind _returnvalue_10 (`|CreateWidget` "/Game/VN_UI/BP_infolink_cutscene.BP_infolink_cutscene_C"))
      (`UserWidget.AddToViewport` _returnvalue_10 0)
      (`/Game/VN_UI/BP_infolink_cutscene.MESSAGE` _returnvalue_10 "/Game/VN_UI/Avatars/T_Infolink_Wizard.T_Infolink_Wizard" "NO! There are zones, none of them is a hill." "Wizard"))
    (:`11`
      (bind _returnvalue_11 (`|CreateWidget` "/Game/VN_UI/BP_infolink_cutscene.BP_infolink_cutscene_C"))
      (`UserWidget.AddToViewport` _returnvalue_11 0)
      (`/Game/VN_UI/BP_infolink_cutscene.MESSAGE` _returnvalue_11 "/Game/VN_UI/Avatars/T_Infolink_Wizard.T_Infolink_Wizard" "Anyways, this is a team mode, so… \nHellsing, Wendy and Commando – you will be Team Blue. The rest are Team Red." "Wizard"))
    (:`12`
      (bind _returnvalue_12 (`|CreateWidget` "/Game/VN_UI/BP_infolink_cutscene.BP_infolink_cutscene_C"))
      (`UserWidget.AddToViewport` _returnvalue_12 0)
      (`/Game/VN_UI/BP_infolink_cutscene.MESSAGE` _returnvalue_12 "/Game/VN_UI/Avatars/T_Infolink_Wizard.T_Infolink_Wizard" "Congratulations! I knew you wouldn’t fail me. Now onto the next match!" "Wizard"))
    (:`13`
      (bind _returnvalue_13 (`|CreateWidget` "/Game/VN_UI/BP_infolink_cutscene.BP_infolink_cutscene_C"))
      (`UserWidget.AddToViewport` _returnvalue_13 0)
      (`/Game/VN_UI/BP_infolink_cutscene.MESSAGE` _returnvalue_13 "/Game/VN_UI/Avatars/T_Infolink_Molly.T_Infolink_Molly" "Well, that sucked." "Molly"))
    (:`14`
      (bind _returnvalue_14 (`|CreateWidget` "/Game/VN_UI/BP_infolink_cutscene.BP_infolink_cutscene_C"))
      (`UserWidget.AddToViewport` _returnvalue_14 0)
      (`/Game/VN_UI/BP_infolink_cutscene.MESSAGE` _returnvalue_14 "/Game/VN_UI/Avatars/T_Infolink_Wizard.T_Infolink_Wizard" "Big time. Now back in you go!" "Wizard"))
    (:`15`
      ;[1 1 1] DOM2
      (bind _returnvalue_15 (`|CreateWidget` "/Game/VN_UI/BP_infolink_cutscene.BP_infolink_cutscene_C")) ; 15
      (`UserWidget.AddToViewport` _returnvalue_15 0)
      (`/Game/VN_UI/BP_infolink_cutscene.MESSAGE` _returnvalue_15 "/Game/VN_UI/Avatars/T_Infolink_Molly.T_Infolink_Molly" "Huh… This doesn’t look like an arena." "Molly"))
    (:`16`
      (bind _returnvalue_16 (`|CreateWidget` "/Game/VN_UI/BP_infolink_cutscene.BP_infolink_cutscene_C"))
      (`UserWidget.AddToViewport` _returnvalue_16 0)
      (`/Game/VN_UI/BP_infolink_cutscene.MESSAGE` _returnvalue_16 "/Game/VN_UI/Avatars/T_Infolink_Wizard.T_Infolink_Wizard" "Stay calm. Everything is under control. The portal… misfired." "Wizard"))
    (:`17`
      (bind _returnvalue_17 (`|CreateWidget` "/Game/VN_UI/BP_infolink_cutscene.BP_infolink_cutscene_C"))
      (`UserWidget.AddToViewport` _returnvalue_17 0)
      (`/Game/VN_UI/BP_infolink_cutscene.MESSAGE` _returnvalue_17 "/Game/VN_UI/Avatars/T_Infolink_Molly.T_Infolink_Molly" "What?" "Molly"))
    (:`18`
      (bind _returnvalue_18 (`|CreateWidget` "/Game/VN_UI/BP_infolink_cutscene.BP_infolink_cutscene_C"))
      (`UserWidget.AddToViewport` _returnvalue_18 0)
      (`/Game/VN_UI/BP_infolink_cutscene.MESSAGE` _returnvalue_18 "/Game/VN_UI/Avatars/T_Infolink_Wizard.T_Infolink_Wizard" "There are some…test levels that have been unplugged for a very long time. \nNo matter, just find the exit and you’ll get back to the lobby." "Wizard"))
    (:`19`
      (bind _returnvalue_19 (`|CreateWidget` "/Game/VN_UI/BP_infolink_cutscene.BP_infolink_cutscene_C"))
      (`UserWidget.AddToViewport` _returnvalue_19 0)
      (`/Game/VN_UI/BP_infolink_cutscene.MESSAGE` _returnvalue_19 "/Game/VN_UI/Avatars/T_Infolink_Molly.T_Infolink_Molly" "What, why did you leave some places incomplete? Hey?" "Molly"))
    (:`20`
      ;[1 1 1] DOM3
      (bind _returnvalue_20 (`|CreateWidget` "/Game/VN_UI/BP_infolink_cutscene.BP_infolink_cutscene_C")) ; 20
      (`UserWidget.AddToViewport` _returnvalue_20 0)
      (`/Game/VN_UI/BP_infolink_cutscene.MESSAGE` _returnvalue_20 "/Game/VN_UI/Avatars/T_Infolink_Hacker.T_Infolink_Hacker" "Enaging hostile at 30% load." "Hacker"))
    (:`21`
      (bind _returnvalue_21 (`|CreateWidget` "/Game/VN_UI/BP_infolink_cutscene.BP_infolink_cutscene_C"))
      (`UserWidget.AddToViewport` _returnvalue_21 0)
      (`/Game/VN_UI/BP_infolink_cutscene.MESSAGE` _returnvalue_21 "/Game/VN_UI/Avatars/T_Infolink_Hacker.T_Infolink_Hacker" "Finally, someone worthy. I started to lose hope. We’ll meet again." "Hacker"))))

(fn `UserConstructionScript`)