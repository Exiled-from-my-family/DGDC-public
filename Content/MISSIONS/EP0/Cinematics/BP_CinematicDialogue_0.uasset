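; Scripted dialogue and music actions for the Episode 0 cinematic, in which a Wizard welcomes a revived Molly to an FPS arena game.
; Dialogue switches on a line number, creating a new skippable BP_infolink_cutscene widget with hardcoded portrait, text and speaker name.
; Music plays one of two EP0 tracks as 2D sound.
; Quit restores the player's HUD and removes the cutscene widgets.
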(event `Music`
  (params (Track :type Integer))
  (bind _returnvalue (`GameplayStatics.SpawnSound2D` (select `int` Track :`0` "/Game/MISSIONS/EP0/Music/SC_EP0_pt1.SC_EP0_pt1" :`1` "/Game/MISSIONS/EP0/Music/SC_EP0_pt2.SC_EP0_pt2" :!type "SoundBase Object Reference") 1.0 1.0 0.0 null))
  (`AudioComponent.Play` _returnvalue 0.0))

(event `Quit`
  (bind _player (`/Game/Blueprints/NewFunctionLibrary.get player`))
  (`Widget.SetVisibility` (`/Game/Blueprints/CHARACTERS/fpsMovementCharacter_light_1_vq3.HUD` _player) "Visible")
  (bind _foundwidgets (`WidgetBlueprintLibrary.GetAllWidgetsOfClass` "/Game/VN_UI/BP_infolink_cutscene.BP_infolink_cutscene_C"))
  (`Widget.RemoveFromParent` _foundwidgets))

(event `Dialogue`
  (params (Line :type Integer :default 1))
  (switch `int` Line
    (:`1`
      (bind _returnvalue (`|CreateWidget` "/Game/VN_UI/BP_infolink_cutscene.BP_infolink_cutscene_C"))
      (`UserWidget.AddToViewport` _returnvalue 0)
      (`/Game/VN_UI/BP_infolink_cutscene.MESSAGE` _returnvalue "/Game/VN_UI/Avatars/noiser.noiser" " I- I’m… back?" " "))
    (:`2`
      (bind _returnvalue_2 (`|CreateWidget` "/Game/VN_UI/BP_infolink_cutscene.BP_infolink_cutscene_C"))
      (`UserWidget.AddToViewport` _returnvalue_2 0)
      (`/Game/VN_UI/BP_infolink_cutscene.MESSAGE` _returnvalue_2 "/Engine/MapTemplates/TilingNoise05.TilingNoise05" "You sure are. Now, just follow the path ahead, you’ll get your questions answered!" " ???"))
    (:`3`
      (bind _returnvalue_3 (`|CreateWidget` "/Game/VN_UI/BP_infolink_cutscene.BP_infolink_cutscene_C"))
      (`UserWidget.AddToViewport` _returnvalue_3 0)
      (`/Game/VN_UI/BP_infolink_cutscene.MESSAGE` _returnvalue_3 "/Game/VN_UI/Avatars/T_Infolink_Wizard.T_Infolink_Wizard" "Welcome!" "Wizard"))
    (:`4`
      (bind _returnvalue_4 (`|CreateWidget` "/Game/VN_UI/BP_infolink_cutscene.BP_infolink_cutscene_C"))
      (`UserWidget.AddToViewport` _returnvalue_4 0)
      (`/Game/VN_UI/BP_infolink_cutscene.MESSAGE` _returnvalue_4 "/Game/VN_UI/Avatars/T_Infolink_Molly.T_Infolink_Molly" "Who are you? What is this place?" " Molly"))
    (:`5`
      (bind _returnvalue_5 (`|CreateWidget` "/Game/VN_UI/BP_infolink_cutscene.BP_infolink_cutscene_C"))
      (`UserWidget.AddToViewport` _returnvalue_5 0)
      (`/Game/VN_UI/BP_infolink_cutscene.MESSAGE` _returnvalue_5 "/Game/VN_UI/Avatars/T_Infolink_Wizard.T_Infolink_Wizard" "This… is a game! An FPS arena to be exact. An elegant genre from a past age. \nModern gamers, well, just lost their touch. No bunny hopping, no rail-flicking, just a mindless, immediate reward." "Wizard"))
    (:`6`
      (bind _returnvalue_6 (`|CreateWidget` "/Game/VN_UI/BP_infolink_cutscene.BP_infolink_cutscene_C"))
      (`UserWidget.AddToViewport` _returnvalue_6 0)
      (`/Game/VN_UI/BP_infolink_cutscene.MESSAGE` _returnvalue_6 "/Game/VN_UI/Avatars/T_Infolink_Wizard.T_Infolink_Wizard" "But! I’ve discovered that through necromancy one can revive a dead medium as well!" "Wizard"))
    (:`7`
      (bind _returnvalue_7 (`|CreateWidget` "/Game/VN_UI/BP_infolink_cutscene.BP_infolink_cutscene_C"))
      (`UserWidget.AddToViewport` _returnvalue_7 0)
      (`/Game/VN_UI/BP_infolink_cutscene.MESSAGE` _returnvalue_7 "/Game/VN_UI/Avatars/T_Infolink_Molly.T_Infolink_Molly" "So, you’re a sorcerer?" "Molly"))
    (:`8`
      (bind _returnvalue_8 (`|CreateWidget` "/Game/VN_UI/BP_infolink_cutscene.BP_infolink_cutscene_C"))
      (`UserWidget.AddToViewport` _returnvalue_8 0)
      (`/Game/VN_UI/BP_infolink_cutscene.MESSAGE` _returnvalue_8 "/Game/VN_UI/Avatars/T_Infolink_Wizard.T_Infolink_Wizard" "Heh! A wizard. Wizard!  \nAnd I summoned you here, because this game needs players. \nAnd you, my dear, are one of them. Now, get into the portal, youl’ll meet the others." "Wizard"))))

(fn `UserConstructionScript`)