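; BP_EP0_Door is an Episode 0 door actor that moves as soon as it begins play, using a tutorial door sound.
; BeginPlay caches the Cube's start location, plays the DoorMovement timeline to offset it from there, fires the sound and enables query and physics collision.
; Each timeline update also calls SetTickableWhenPaused.
; The Box overlap event is empty, so nothing triggers on overlap.
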(event `self.ReceiveBeginPlay`
  (bind _returnvalue (`SceneComponent.K2_GetComponentLocation` (`self.Cube`)))
  (`|ExecutionSequence`
    (:`then_0`
      (set `self.DoorStartLocation` _returnvalue))
    (:`then_1`
      (bind (_direction _newtrack_2) (`Timeline|DoorMovement`)
        (:`Update`
          (`self.SetTickableWhenPaused` true)
          (`SceneComponent.K2_SetWorldLocation` (`self.Cube`) (+ _newtrack_2 (`self.DoorStartLocation`)) false false))))
    (:`then_2`
      (`GameplayStatics.PlaySoundAtLocation` "/Game/MISSIONS/EP0/Audio/SC_TutorialDoor.SC_TutorialDoor" _returnvalue (struct) 1.0 1.0 0.0 null null null))
    (:`then_3`
      (`PrimitiveComponent.SetCollisionEnabled` (`self.Cube`) "QueryAndPhysics"))))

(event `self.Box.OnComponentBeginOverlap`
  (params (OverlappedComponent :type "PrimitiveComponent Object Reference") (OtherActor :type "Actor Object Reference") (OtherComp :type "PrimitiveComponent Object Reference") (OtherBodyIndex :type Integer) (bFromSweep :type Boolean) (SweepResult :type "HitResult Structure (by ref)")))

(fn `UserConstructionScript`)