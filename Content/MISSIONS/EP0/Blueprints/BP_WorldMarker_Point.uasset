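; World marker actor for a capturable point in an EP0 mission, showing a widget that reflects the owning team.
; BeginPlay applies text, color and arrow visibility through a UI_WorldMarker cast.
; Tick scales the UI_WorldMarker_Point border by player distance, larger when close, using a clamped lerp.
; Team_RED, Team_BLUE and Team_NONE events tint that border red, blue or white.
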(event `self.ReceiveBeginPlay`
  (bind _asui_world_marker (cast `/Game/Blueprints/UI/UI_WorldMarker` (`WidgetComponent.GetUserWidgetObject` (`self.Widget`))))
  (set `/Game/Blueprints/UI/UI_WorldMarker.Text` (`self.WidgetText`) _asui_world_marker)
  (set `/Game/Blueprints/UI/UI_WorldMarker.text color` (make `SlateColor` (`self.WidgetColor`)) _asui_world_marker)
  (`Widget.SetVisibility` (`/Game/Blueprints/UI/UI_WorldMarker.TextBlock` _asui_world_marker) (select `bool` (`self.ArrowVisible`) :`false` "Hidden" :`true` "Visible" :!type "ESlateVisibility Enum")))

(event `self.ReceiveTick`
  (params (DeltaSeconds :type "Float (single-precision)"))
  (bind _returnvalue (`KismetMathLibrary.FClamp` (`KismetMathLibrary.Lerp` 3.0 1.0 (`KismetMathLibrary.FClamp` (/ (`KismetMathLibrary.Vector_Distance` (`self.K2_GetActorLocation` (`GameplayStatics.GetPlayerCharacter` 0)) (`self.K2_GetActorLocation`)) 1000.0) 0.5 5.0)) 1.0 3.0))
  (bind _asui_world_marker_point (cast `/Game/Blueprints/UI/UI_WorldMarker_Point` (`WidgetComponent.GetUserWidgetObject` (`self.Widget`))))
  (`Widget.SetRenderScale` (`/Game/Blueprints/UI/UI_WorldMarker_Point.Border_93` _asui_world_marker_point) (`KismetMathLibrary.MakeVector2D` _returnvalue _returnvalue)))

(event `Team_RED`
  ;[1 1 1] Change color depending on which team captured point
  (bind _asui_world_marker_point (cast `/Game/Blueprints/UI/UI_WorldMarker_Point` (`WidgetComponent.GetUserWidgetObject` (`self.Widget`))))
  (`Border.SetContentColorAndOpacity` (`/Game/Blueprints/UI/UI_WorldMarker_Point.Border_93` _asui_world_marker_point) (struct :`R` 1.0 :`G` 0.02 :`A` 1.0)))

(event `Team_BLUE`
  ;[1 1 1] Change color depending on which team captured point
  (bind _asui_world_marker_point (cast `/Game/Blueprints/UI/UI_WorldMarker_Point` (`WidgetComponent.GetUserWidgetObject` (`self.Widget`))))
  (`Border.SetContentColorAndOpacity` (`/Game/Blueprints/UI/UI_WorldMarker_Point.Border_93` _asui_world_marker_point) (struct :`R` 0.2 :`G` 0.333333 :`B` 1.0 :`A` 1.0)))

(event `Team_NONE`
  ;[1 1 1] Change color depending on which team captured point
  (bind _asui_world_marker_point (cast `/Game/Blueprints/UI/UI_WorldMarker_Point` (`WidgetComponent.GetUserWidgetObject` (`self.Widget`))))
  (`Border.SetContentColorAndOpacity` (`/Game/Blueprints/UI/UI_WorldMarker_Point.Border_93` _asui_world_marker_point) (struct :`R` 1.0 :`G` 1.0 :`B` 1.0 :`A` 1.0)))

(fn `UserConstructionScript`)