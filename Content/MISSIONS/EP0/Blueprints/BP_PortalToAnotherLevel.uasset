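; A level portal: when the living player character enters its box, it loads another map.
; The overlap zeroes the character's gravity, slows global time and starts a camera fade, then plays an optional sound and shows a loading screen widget.
; After short delays it opens the revisit map if the configured unlockable is owned, marking the default map as won, otherwise the default map.
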(event `self.Box.OnComponentBeginOverlap`
  (params (OverlappedComponent :type "PrimitiveComponent Object Reference") (OtherActor :type "Actor Object Reference") (OtherComp :type "PrimitiveComponent Object Reference") (OtherBodyIndex :type Integer) (bFromSweep :type Boolean) (SweepResult :type "HitResult Structure (by ref)"))
  (bind _sound (`self.sound`))
  (bind _asfps_movement_character_light_1_vq_3 (cast `/Game/Blueprints/CHARACTERS/fpsMovementCharacter_light_1_vq3` OtherActor))
  (set `CharacterMovementComponent.GravityScale` 0.0 (`Character.CharacterMovement` _asfps_movement_character_light_1_vq_3))
  (if (not (`/Game/Blueprints/CHARACTERS/fpsMovementCharacter_light_1_vq3.IsDead?` _asfps_movement_character_light_1_vq_3))
    (`GameplayStatics.SetGlobalTimeDilation` 0.1)
    (`PlayerCameraManager.StartCameraFade` :`self` (`GameplayStatics.GetPlayerCameraManager` 0) :`ToAlpha` 1.0 :`Duration` 0.5 :`bShouldFadeAudio` (not (`KismetSystemLibrary.IsValid` _sound)) :`bHoldWhenFinished` true)
    (`KismetSystemLibrary.Delay` 0.05)
    (`/Engine/EditorBlueprintResources/StandardMacros.IsValid` _sound
      (:`Is Valid`
        (`GameplayStatics.PlaySound2D` _sound 1.0 1.0 0.0 null null))
      (:`Is Not Valid`
        _))
    (bind _returnvalue (`|CreateWidget` "/Game/Blueprints/UI/UI_LoadingScreen.UI_LoadingScreen_C"))
    (`UserWidget.AddToViewport` _returnvalue 5)
    (`KismetSystemLibrary.Delay` 0.1)
    ;[1 1 1] Portal sends player to different map if he won the match
    (bind _unlocked_ (`/Game/Blueprints/NewFunctionLibrary.has unlockable` (`self.Unlockable`)))
    (if _unlocked_
      (`GameplayStatics.OpenLevel` (`self.map name revisit`)) ; Destination if default map is won
      (else
        (`GameplayStatics.OpenLevel` (`self.map name`)) ; Default destination
      ))))

(fn `UserConstructionScript`)