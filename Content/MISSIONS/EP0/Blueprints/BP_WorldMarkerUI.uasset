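; BP_WorldMarkerUI is a world marker Blueprint that displays a UI_WorldMarker widget with configurable text and color.
; On BeginPlay it casts its Widget component's user widget to UI_WorldMarker and copies WidgetText and WidgetColor into it.
; The ArrowVisible flag shows or hides the widget's TextBlock element.
; Setup runs once at start, with no construction script logic or runtime updates.
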(event `self.ReceiveBeginPlay`
  (bind _asui_world_marker (cast `/Game/Blueprints/UI/UI_WorldMarker` (`WidgetComponent.GetUserWidgetObject` (`self.Widget`))))
  (set `/Game/Blueprints/UI/UI_WorldMarker.Text` (`self.WidgetText`) _asui_world_marker)
  (set `/Game/Blueprints/UI/UI_WorldMarker.text color` (make `SlateColor` (`self.WidgetColor`)) _asui_world_marker)
  (`Widget.SetVisibility` (`/Game/Blueprints/UI/UI_WorldMarker.TextBlock` _asui_world_marker) (select `bool` (`self.ArrowVisible`) :`false` "Hidden" :`true` "Visible" :!type "ESlateVisibility Enum")))

(fn `UserConstructionScript`)