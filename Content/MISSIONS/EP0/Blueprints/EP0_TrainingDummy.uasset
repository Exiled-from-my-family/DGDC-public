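; Training dummy actor for the EP0 mission, built on a parent class that supplies its health bar and death state.
; Shortly after BeginPlay it overrides the dodge damage threshold with a high value.
; Tick polls IsDead and, once, notifies the health bar, toggles mesh visibility, calls CallDummyDied, then destroys the actor after a short delay.
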(event `self.ReceiveBeginPlay`
  (`parent.ReceiveBeginPlay`)
  (`KismetSystemLibrary.Delay` 0.2)
  (set `self.Dodge dmg threshold` 1000.0))

(event `self.ReceiveTick`
  (params (DeltaSeconds :type "Float (single-precision)"))
  (if (`self.IsDead?`)
    (`/Engine/EditorBlueprintResources/StandardMacros.DoOnce` false
      (:`Completed`
        (`/Game/Blueprints/HEALTHBARS/Blueprints/Widgets/Widget_FloatingHealthbar.OnParentActorDead` (`self.Get Healthbar`))
        (`SceneComponent.ToggleVisibility` (`self.Mesh`) true)
        (`self.DummyDied`)
        (`KismetSystemLibrary.Delay` 0.3)
        (`self.K2_DestroyActor`)))))

(fn `UserConstructionScript`
  (`parent.UserConstructionScript`))