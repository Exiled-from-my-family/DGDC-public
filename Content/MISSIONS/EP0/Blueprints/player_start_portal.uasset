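; Player start marker for portals that labels itself with the map names of a linked Portal.
; The construction script copies the map name from Portal when it is valid and shows it on one text render.
; A second text render shows the Portal's revisit map name, which is read outside the validity check.
; The event graph holds no active logic.
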(fn `UserConstructionScript`
  (bind _portal (`self.portal`))
  (`/Engine/EditorBlueprintResources/StandardMacros.IsValid` _portal
    (:`Is Valid`
      (bind _output_get (set `self.map name` (`/Game/MISSIONS/EP0/Blueprints/BP_PortalToAnotherLevel.map name` _portal))))
    (:`Is Not Valid`
      _))
  (`TextRenderComponent.K2_SetText` (`self.TextRender`) (`KismetTextLibrary.Conv_NameToText` _output_get))
  (bind _output_get_2 (set `self.revisit` (`/Game/MISSIONS/EP0/Blueprints/BP_PortalToAnotherLevel.map name revisit` _portal)))
  (`TextRenderComponent.K2_SetText` (`self.TextRender1`) (`KismetTextLibrary.Conv_NameToText` _output_get_2)))