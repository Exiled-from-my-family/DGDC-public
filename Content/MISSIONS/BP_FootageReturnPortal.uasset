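; Portal Blueprint that, going by its name and logic, returns the player to the map their headcam footage came from.
; Shortly after BeginPlay it checks SetHeadcamFootage and, on success, takes its destination MapName from the game instance's stored HeadcamFootageFromThisMap.
; Construction only sets a placeholder for MapNameRevisit, whose instance-based assignment is left unwired; any travel behavior is not in this graph.
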(event `self.ReceiveBeginPlay`
  (`parent.ReceiveBeginPlay`)
  (`KismetSystemLibrary.Delay` 0.2)
  (if (`/Game/Blueprints/NewFunctionLibrary.set headcam footage`)
    (set `self.map name` (`/Game/Blueprints/DeadGaemInstance.headcam footage from this map` (`/Game/Blueprints/NewFunctionLibrary.dead game instance PURE`)))))

(fn `UserConstructionScript`
  (`parent.UserConstructionScript`)
  (set `self.map name revisit` "CHANGED BY INSTANCE"))