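; Episode 4 cinematic dialogue Blueprint that shows infolink cutscene messages from Molly, the CEO and the Hacker.
; Each scene event (casino intro, barrier, recon team) switches on a Line index to pick hardcoded dialogue.
; Each line spawns a new skippable BP_infolink_cutscene widget and passes it portrait, text and speaker name.
; Quit makes the player HUD visible again and removes top-level infolink cutscene widgets from the screen.
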(event `Quit`
  (bind _player (`/Game/Blueprints/NewFunctionLibrary.get player`))
  (`Widget.SetVisibility` (`/Game/Blueprints/CHARACTERS/fpsMovementCharacter_light_1_vq3.HUD` _player) "Visible")
  (bind _foundwidgets (`WidgetBlueprintLibrary.GetAllWidgetsOfClass` "/Game/VN_UI/BP_infolink_cutscene.BP_infolink_cutscene_C"))
  (`Widget.RemoveFromParent` _foundwidgets))

(event `Dialogue Casino intro`
  (params (Line :type Integer :default 1))
  (switch `int` Line
    (:`0`
      (bind _returnvalue (`|CreateWidget` "/Game/VN_UI/BP_infolink_cutscene.BP_infolink_cutscene_C")) ; 0
      (`UserWidget.AddToViewport` _returnvalue 0)
      (`/Game/VN_UI/BP_infolink_cutscene.MESSAGE` _returnvalue "/Game/VN_UI/Avatars/T_Infolink_Molly.T_Infolink_Molly" "Whoa, easy boys, is this how you treat a lady?" "Molly"))
    (:`1`
      (bind _returnvalue_2 (`|CreateWidget` "/Game/VN_UI/BP_infolink_cutscene.BP_infolink_cutscene_C")) ; 1
      (`UserWidget.AddToViewport` _returnvalue_2 0)
      (`/Game/VN_UI/BP_infolink_cutscene.MESSAGE` _returnvalue_2 "/Game/VN_UI/Avatars/T_Infolink_CEO.T_Infolink_CEO" "I only see a test subject." "CEO"))
    (:`2`
      (bind _returnvalue_3 (`|CreateWidget` "/Game/VN_UI/BP_infolink_cutscene.BP_infolink_cutscene_C"))
      (`UserWidget.AddToViewport` _returnvalue_3 0)
      (`/Game/VN_UI/BP_infolink_cutscene.MESSAGE` _returnvalue_3 "/Game/VN_UI/Avatars/T_Infolink_CEO.T_Infolink_CEO" "See, I would’ve handled things differently,  but at least my son proved to be useful in completing our research." "CEO"))
    (:`3`
      (bind _returnvalue_4 (`|CreateWidget` "/Game/VN_UI/BP_infolink_cutscene.BP_infolink_cutscene_C"))
      (`UserWidget.AddToViewport` _returnvalue_4 0)
      (`/Game/VN_UI/BP_infolink_cutscene.MESSAGE` _returnvalue_4 "/Game/VN_UI/Avatars/T_Infolink_Molly.T_Infolink_Molly" "Your...son?" "Molly"))
    (:`4`
      (bind _returnvalue_5 (`|CreateWidget` "/Game/VN_UI/BP_infolink_cutscene.BP_infolink_cutscene_C"))
      (`UserWidget.AddToViewport` _returnvalue_5 0)
      (`/Game/VN_UI/BP_infolink_cutscene.MESSAGE` _returnvalue_5 "/Game/VN_UI/Avatars/T_Infolink_CEO.T_Infolink_CEO" "Yes. I made the mistake of raising him a bit too spoiled so he feels entitled to whatever he wants at that moment. He used the security clearance I gave him to access our research, got his hands on a bunch of old weapon prototypes, and voila." "CEO"))
    (:`5`
      (bind _returnvalue_6 (`|CreateWidget` "/Game/VN_UI/BP_infolink_cutscene.BP_infolink_cutscene_C"))
      (`UserWidget.AddToViewport` _returnvalue_6 0)
      (`/Game/VN_UI/BP_infolink_cutscene.MESSAGE` _returnvalue_6 "/Game/VN_UI/Avatars/T_Infolink_CEO.T_Infolink_CEO" "His passion seems to have guided him to the missing link: cutting edge technology fused with old magic. A digital version of the dead. We aren’t sure of what your lot is, yet, but I am rather certain that entities who cannot die are enough for kicking off a new era of bloodsports entertainment." "CEO"))
    (:`6`
      (bind _returnvalue_7 (`|CreateWidget` "/Game/VN_UI/BP_infolink_cutscene.BP_infolink_cutscene_C"))
      (`UserWidget.AddToViewport` _returnvalue_7 0)
      (`/Game/VN_UI/BP_infolink_cutscene.MESSAGE` _returnvalue_7 "/Game/VN_UI/Avatars/T_Infolink_Molly.T_Infolink_Molly" "You have to be kidding me." "Molly"))
    (:`7`
      (bind _returnvalue_8 (`|CreateWidget` "/Game/VN_UI/BP_infolink_cutscene.BP_infolink_cutscene_C"))
      (`UserWidget.AddToViewport` _returnvalue_8 0)
      (`/Game/VN_UI/BP_infolink_cutscene.MESSAGE` _returnvalue_8 "/Game/VN_UI/Avatars/T_Infolink_CEO.T_Infolink_CEO" "Oh, no. While he pursued things like raising the dead and summoning demons for nostalgia’s sake, I conversed with a socratic daemon of pure logic. This was the result." "CEO"))
    (:`8`
      (bind _returnvalue_9 (`|CreateWidget` "/Game/VN_UI/BP_infolink_cutscene.BP_infolink_cutscene_C"))
      (`UserWidget.AddToViewport` _returnvalue_9 0)
      (`/Game/VN_UI/BP_infolink_cutscene.MESSAGE` _returnvalue_9 "/Game/VN_UI/Avatars/T_Infolink_Molly.T_Infolink_Molly" "I see where he took his self importance from…" "Molly"))
    (:`9`
      (bind _returnvalue_10 (`|CreateWidget` "/Game/VN_UI/BP_infolink_cutscene.BP_infolink_cutscene_C"))
      (`UserWidget.AddToViewport` _returnvalue_10 0)
      (`/Game/VN_UI/BP_infolink_cutscene.MESSAGE` _returnvalue_10 "/Game/VN_UI/Avatars/T_Infolink_CEO.T_Infolink_CEO" "Add her to the test routine, I’ll check the results from my office; no reason for me to stay and monitor the situation from here any longer." "CEO"))
    (:`10`
      (bind _returnvalue_11 (`|CreateWidget` "/Game/VN_UI/BP_infolink_cutscene.BP_infolink_cutscene_C"))
      (`UserWidget.AddToViewport` _returnvalue_11 0)
      (`/Game/VN_UI/BP_infolink_cutscene.MESSAGE` _returnvalue_11 "/Game/VN_UI/Avatars/T_Infolink_Hacker.T_Infolink_Hacker" "Play along, I need some time to gather as much evidence as possible." "Hacker"))))

(event `Dialogue Barrier`
  (params (Line :type Integer :default 1))
  (switch `int` Line
    (:`0`
      (bind _returnvalue (`|CreateWidget` "/Game/VN_UI/BP_infolink_cutscene.BP_infolink_cutscene_C")) ; 0
      (`UserWidget.AddToViewport` _returnvalue 0)
      (`/Game/VN_UI/BP_infolink_cutscene.MESSAGE` _returnvalue "/Game/VN_UI/Avatars/T_Infolink_Hacker.T_Infolink_Hacker" "They have sealed their entrance behind a firewall of sorts. Try to find a way to bypass it." "Hacker"))))

(event `Dialogue recon team`
  (params (Line :type Integer :default 1))
  (switch `int` Line
    (:`0`
      (bind _returnvalue (`|CreateWidget` "/Game/VN_UI/BP_infolink_cutscene.BP_infolink_cutscene_C")) ; 0
      (`UserWidget.AddToViewport` _returnvalue 0)
      (`/Game/VN_UI/BP_infolink_cutscene.MESSAGE` _returnvalue "/Game/VN_UI/Avatars/T_Infolink_Hacker.T_Infolink_Hacker" "Galactamax has probably taken interest in the Wizard's experiments after they watched the security footage of the Island." "Hacker"))
    (:`1`
      (bind _returnvalue_2 (`|CreateWidget` "/Game/VN_UI/BP_infolink_cutscene.BP_infolink_cutscene_C")) ; 1
      (`UserWidget.AddToViewport` _returnvalue_2 0)
      (`/Game/VN_UI/BP_infolink_cutscene.MESSAGE` _returnvalue_2 "/Game/VN_UI/Avatars/T_Infolink_Hacker.T_Infolink_Hacker" "The recon team is heading down there, they must have set up a link on their end to get free access to the place. I believe that's where your friends ended up." "Hacker"))))

(fn `UserConstructionScript`)