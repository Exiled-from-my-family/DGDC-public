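; BP_Office_Monitor is a breakable computer monitor prop for an Episode 4 mission.
; The first damage event of any kind passes a DoOnce that swaps the mesh to a broken-screen material and prints a debug "Hello".
; It also spawns smoke, sparks and a robot gib sound at an offset from the mesh.
; A check limiting damage to "Projectile"-tagged causers exists but is disconnected.
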(event `self.ReceiveAnyDamage`
  (params (Damage :type "Float (single-precision)") (DamageType :type "DamageType Object Reference") (InstigatedBy :type "Controller Object Reference") (DamageCauser :type "Actor Object Reference"))
  (bind _sm_computer_a (`self.SM_Computer_A`))
  (bind _returnvalue (+ (`SceneComponent.K2_GetComponentLocation` _sm_computer_a) (`self.VFX location`)))
  (`/Engine/EditorBlueprintResources/StandardMacros.DoOnce` false
    (:`Completed`
      (`PrimitiveComponent.SetMaterial` _sm_computer_a 1 "/Game/MATERIALS/M_BrokenMonitor.M_BrokenMonitor")
      (`GameplayStatics.SpawnEmitterAtLocation` "/Game/StylizedNatureVol2/Effects/P_Stylized_Smoke.P_Stylized_Smoke" _returnvalue)
      (`GameplayStatics.SpawnEmitterAtLocation` "/Game/kosm_fps_assets/Misc/Particles/P_Sparks1.P_Sparks1" _returnvalue (struct) (0.25 0.25 0.25))
      (`GameplayStatics.SpawnSoundAtLocation` "/Game/AUDIO/SFX_Damage/SC_Gibs_Robot.SC_Gibs_Robot" _returnvalue (struct) 1.0 1.0 0.0 null null)
      (`KismetSystemLibrary.PrintString` "Hello"))))

(fn `UserConstructionScript`)