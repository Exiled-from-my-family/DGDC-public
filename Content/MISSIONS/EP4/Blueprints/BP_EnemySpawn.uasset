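; Enemy spawn point for EP4 missions whose sphere and arrow markers stay hidden until its DOthespawning event fires.
; The event reveals and grows the sphere via timeline while optional FullVFX plays teleport particles and sounds, with a delay before the enemy appears.
; It spawns the configured EnemyType above the point, yawed toward the player, assigns TagsToAdd, then destroys itself shortly after.
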(event `self.ReceiveBeginPlay`
  (`SceneComponent.SetVisibility` (`self.Sphere`) false false)
  (`SceneComponent.SetVisibility` (`self.Arrow`) false false))

(event `DO the spawning`
  (bind _returnvalue_location (`KismetMathLibrary.BreakTransform` (`self.GetTransform`)))
  (bind (_returnvalue_roll _returnvalue_pitch _returnvalue_yaw) (`KismetMathLibrary.BreakRotator` (`KismetMathLibrary.FindLookAtRotation` (`self.K2_GetActorLocation`) (`self.K2_GetActorLocation` (`GameplayStatics.GetPlayerCharacter` 0)))))
  (`self.SetActorHiddenInGame` false)
  (`SceneComponent.SetVisibility` (`self.Sphere`) true false)
  (`SceneComponent.SetVisibility` (`self.Arrow`) true false)
  (`|ExecutionSequence`
    (:`then_0`
      (if (`self.Full VFX?`)
        (`GameplayStatics.SpawnEmitterAtLocation` "/Game/rpgeffects/Particles/P_Mage_MagicSphere.P_Mage_MagicSphere" (+ (`self.K2_GetActorLocation`) (0.0 0.0 5.0)))
        (`GameplayStatics.PlaySoundAtLocation` "/Game/AUDIO/SFX_UI/SW_Teleporter_Magic_Rev.SW_Teleporter_Magic_Rev" (`self.K2_GetActorLocation`) (struct) 0.8 1.0 0.0 "/Game/kosm_fps_assets/Misc/SoundFX/SoundAttenuationPickup.SoundAttenuationPickup" null null)
        (`KismetSystemLibrary.Delay` 1.0)
        (`GameplayStatics.SpawnEmitterAtLocation` "/Game/rpgeffects/Particles/P_Warrior_HeavyImpact.P_Warrior_HeavyImpact" (+ (`self.K2_GetActorLocation`) (0.0 0.0 5.0)) (struct) (2.0 2.0 2.0))
        (`GameplayStatics.PlaySoundAtLocation` "/Game/AUDIO/SFX_UI/SW_Teleporter_Tech.SW_Teleporter_Tech" (`self.K2_GetActorLocation`) (struct) 1.0 1.0 0.0 "/Game/kosm_fps_assets/Misc/SoundFX/SoundAttenuationPickup.SoundAttenuationPickup" null null)
        (`GameplayStatics.PlaySoundAtLocation` "/Game/AUDIO/SFX_UI/SW_Teleporter.SW_Teleporter" (`self.K2_GetActorLocation`) (struct) 0.6 1.0 0.0 "/Game/kosm_fps_assets/Misc/SoundFX/SoundAttenuationPickup.SoundAttenuationPickup" null null))
      (bind _returnvalue (`|SpawnActorFromClass` (`self.Enemy type`) (`KismetMathLibrary.MakeTransform` (+ _returnvalue_location (0.0 0.0 100.0)) (`KismetMathLibrary.MakeRotator` 0.0 0.0 _returnvalue_yaw)) "AlwaysSpawn" "OverrideRootScale" null null))
      (set `Actor.Tags` (`self.Tags to add`) _returnvalue)
      (`KismetSystemLibrary.Delay` 0.2)
      (`self.K2_DestroyActor`))
    (:`then_1`
      (bind (_direction _newtrack_0) (`Timeline|Timeline_0` :!via `PlayFromStart`)
        (:`Update`
          (`SceneComponent.SetRelativeScale3D` (`self.Sphere`) (`KismetMathLibrary.VLerp` (0.0 0.0 0.0) (8.0 8.0 8.0) _newtrack_0)))))))

(fn `UserConstructionScript`)