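; BP_Sodacan is a soda can projectile that launches with a random arc, tilt and one of five can materials on spawn, then destroys itself after a fixed lifetime.
; Projectile movement carries the initial flight.
; On bounce it plays a can sound and reports a noise event at the impact, then after a short delay switches the mesh to physics simulation.
; The component hit event is empty.
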(event `self.ReceiveBeginPlay`
  (bind _sodacan (`self.Sodacan`))
  (`ProjectileMovementComponent.SetVelocityInLocalSpace` (`self.ProjectileMovement`) (`KismetMathLibrary.MakeVector` (`KismetMathLibrary.RandomFloatInRange` 350.0 750.0) (`KismetMathLibrary.RandomFloatInRange` -90.0 90.0) (`KismetMathLibrary.RandomFloatInRange` 400.0 850.0)))
  (`SceneComponent.K2_SetRelativeRotation` _sodacan (`KismetMathLibrary.MakeRotator` (`KismetMathLibrary.RandomFloatInRange` -15.0 15.0) (`KismetMathLibrary.RandomFloatInRange` -45.0 45.0)) false false)
  (`PrimitiveComponent.SetMaterial` _sodacan 0 (select `int` (`KismetMathLibrary.RandomIntegerInRange` 0 4) :`0` "/Game/MISSIONS/EP3/Meshes/Materials/M_SodaCan1.M_SodaCan1" :`1` "/Game/MISSIONS/EP3/Meshes/Materials/M_SodaCan2.M_SodaCan2" :`2` "/Game/MISSIONS/EP3/Meshes/Materials/M_SodaCan3.M_SodaCan3" :`3` "/Game/MISSIONS/EP3/Meshes/Materials/M_SodaCan4.M_SodaCan4" :`4` "/Game/MISSIONS/EP3/Meshes/Materials/M_SodaCan5.M_SodaCan5" :!type "MaterialInterface Object Reference"))
  (`KismetSystemLibrary.Delay` 15.0)
  (`self.K2_DestroyActor`))

(event `self.ProjectileMovement.OnProjectileBounce`
  (params (ImpactResult :type "HitResult Structure (by ref)") (ImpactVelocity :type "Vector Structure (by ref)"))
  (bind _returnvalue (`self.K2_GetActorLocation`))
  (`GameplayStatics.PlaySoundAtLocation` "/Game/AUDIO/SC_Can.SC_Can" _returnvalue (struct) 1.0 1.0 0.0 null null null)
  (`AISense_Hearing.ReportNoiseEvent` _returnvalue 1.0 null 1000.0)
  (`KismetSystemLibrary.Delay` 0.5)
  (`PrimitiveComponent.SetSimulatePhysics` (`self.Sodacan`) true))

(event `self.Sodacan.OnComponentHit`
  (params (HitComponent :type "PrimitiveComponent Object Reference") (OtherActor :type "Actor Object Reference") (OtherComp :type "PrimitiveComponent Object Reference") (NormalImpulse :type "Vector Structure") (Hit :type "HitResult Structure (by ref)")))

(fn `UserConstructionScript`)