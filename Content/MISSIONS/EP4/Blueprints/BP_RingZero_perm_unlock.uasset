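; Permanent-unlock pickup for the Ring Zero secondary ability, which destroys itself on BeginPlay if RING0 is already unlocked.
; The first player overlap adds the unlockable, equips it through the GameInstance's AdminTool, sets RailgunAmmo, hides the pickup and plays a sound.
; It shows a pickup message, then after a delay a tutorial widget with the bound Ability 2 key substituted into the text, and destroys itself.
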(event `self.Box.OnComponentBeginOverlap`
  (params (OverlappedComponent :type "PrimitiveComponent Object Reference") (OtherActor :type "Actor Object Reference") (OtherComp :type "PrimitiveComponent Object Reference") (OtherBodyIndex :type Integer) (bFromSweep :type Boolean) (SweepResult :type "HitResult Structure (by ref)"))
  (bind _returnvalue (`GameplayStatics.GetPlayerController` 0))
  (bind _asfps_movement_character_light_1_vq_3 (cast `/Game/Blueprints/CHARACTERS/fpsMovementCharacter_light_1_vq3` OtherActor))
  (`/Engine/EditorBlueprintResources/StandardMacros.DoOnce` false
    (:`Completed`
      (`/Game/Blueprints/NewFunctionLibrary.add unlockable` "RING0")
      (bind _game_instance (`/Game/Blueprints/NewFunctionLibrary.dead game instance`))
      (set `/Game/Blueprints/DeadGaemInstance.admin tool` "NewEnumerator2" _game_instance)
      (set `/Game/Blueprints/CHARACTERS/fpsMovementCharacter_light_1_vq3.RailgunAmmo` 10 _asfps_movement_character_light_1_vq_3)
      (`SceneComponent.SetVisibility` (`self.mesh`) false false)
      (`SceneComponent.SetVisibility` (`self.Cube`) false false)
      (`SceneComponent.SetVisibility` (`self.Cube1`) false false)
      (`SceneComponent.SetVisibility` (`self.PointLight`) false false)
      (`GameplayStatics.PlaySoundAtLocation` "/Game/AUDIO/SFX_UI/SW_Ability_Unlocked.SW_Ability_Unlocked" (`self.K2_GetActorLocation`) (struct) 1.0 1.0 0.0 null null null)
      (bind _returnvalue_2 (`|CreateWidget` "/Game/Blueprints/UI/UI_Pickups/UI_Pickup_Gen_Weapon.UI_Pickup_Gen_Weapon_C"))
      (set `/Game/Blueprints/UI/UI_Pickups/UI_Pickup_Gen_Weapon.Message` "Ring Zero" _returnvalue_2)
      (`UserWidget.AddToViewport` _returnvalue_2 0)
      (`KismetSystemLibrary.Delay` 1.5)
      (bind _returnvalue_3 (`|CreateWidget` "/Game/Blueprints/UI/UI_PauseTutorials/W_PauseTutorialGeneric.W_PauseTutorialGeneric_C" _returnvalue true 0.5))
      (set `/Game/Blueprints/UI/UI_PauseTutorials/W_PauseTutorialGeneric.Message` (`KismetTextLibrary.Conv_StringToText` (`KismetStringLibrary.Replace` " \nYou have obtained the Ring Zero.  \n \nThis counts as a secondary ability, which means it can be equipped by pressing [SHIFT]. \nYour secondary ability is now automatically set to the Ring Zero, if you had another one equipped before, that has been replaced until you change it back in the main menu or at a save station. \n \nActivating it grants temporary invincibility, allowing you to bypass firewalls and barriers at the cost of being unable to shoot. This ability can activated only a limited number of times." "[SHIFT]" (`KismetStringLibrary.Concat_StrStr` "[" (`KismetTextLibrary.Conv_TextToString` (`/Game/Blueprints/NewFunctionLibrary.gamepad or keyboard func` (`InputSettings.GetActionMappingByName` (`InputSettings.GetInputSettings`) "Ability 2"))) "]") "CaseSensitive")) _returnvalue_3)
      (`UserWidget.AddToViewport` _returnvalue_3 0)
      (`WidgetBlueprintLibrary.SetInputMode_GameAndUIEx` _returnvalue _returnvalue_3 "DoNotLock" false)
      (set `PlayerController.bShowMouseCursor` true _returnvalue)
      (`GameplayStatics.PlaySound2D` "/Game/AUDIO/SFX_Pickups/SC_Keycard.SC_Keycard" 0.75 0.6 0.06 null null)
      (`KismetSystemLibrary.Delay` 1.0)
      (`self.K2_DestroyActor`))))

(event `self.ReceiveBeginPlay`
  (bind _unlocked_ (`/Game/Blueprints/NewFunctionLibrary.has unlockable` "RING0"))
  (if _unlocked_
    (`self.K2_DestroyActor`)))

(fn `UserConstructionScript`)