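; One-time pickup that permanently grants the "KNIFE" unlockable, removing itself at BeginPlay if already unlocked.
; When the player character overlaps its box, it registers the unlock, hides its mesh and light, and plays a sound.
; It shows a pickup widget labelled "Ring Zero", then a delayed knife flavour-text popup with mouse cursor, before destroying itself.
; An unconnected Ring Zero tutorial string with key-binding substitution remains in the graph.
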(event `self.Box.OnComponentBeginOverlap`
  (params (OverlappedComponent :type "PrimitiveComponent Object Reference") (OtherActor :type "Actor Object Reference") (OtherComp :type "PrimitiveComponent Object Reference") (OtherBodyIndex :type Integer) (bFromSweep :type Boolean) (SweepResult :type "HitResult Structure (by ref)"))
  (bind _returnvalue (`GameplayStatics.GetPlayerController` 0))
  (cast `/Game/Blueprints/CHARACTERS/fpsMovementCharacter_light_1_vq3` OtherActor)
  (`/Engine/EditorBlueprintResources/StandardMacros.DoOnce` false
    (:`Completed`
      (`/Game/Blueprints/NewFunctionLibrary.add unlockable` "KNIFE")
      (`/Game/Blueprints/NewFunctionLibrary.dead game instance`)
      (`SceneComponent.SetVisibility` (`self.mesh`) false false)
      (`SceneComponent.SetVisibility` (`self.PointLight`) false false)
      (`GameplayStatics.PlaySoundAtLocation` "/Game/AUDIO/SFX_UI/SW_Ability_Unlocked.SW_Ability_Unlocked" (`self.K2_GetActorLocation`) (struct) 1.0 1.0 0.0 null null null)
      (bind _returnvalue_2 (`|CreateWidget` "/Game/Blueprints/UI/UI_Pickups/UI_Pickup_Gen_Weapon.UI_Pickup_Gen_Weapon_C"))
      (set `/Game/Blueprints/UI/UI_Pickups/UI_Pickup_Gen_Weapon.Message` "Ring Zero" _returnvalue_2)
      (`UserWidget.AddToViewport` _returnvalue_2 0)
      (`KismetSystemLibrary.Delay` 1.5)
      (bind _returnvalue_3 (`|CreateWidget` "/Game/Blueprints/UI/UI_PauseTutorials/W_PauseTutorialGeneric.W_PauseTutorialGeneric_C" _returnvalue true 0.5))
      (set `/Game/Blueprints/UI/UI_PauseTutorials/W_PauseTutorialGeneric.Message` "You pick up a strange knife, you might've seen it somewhere else..." _returnvalue_3)
      (`UserWidget.AddToViewport` _returnvalue_3 0)
      (`WidgetBlueprintLibrary.SetInputMode_GameAndUIEx` _returnvalue _returnvalue_3 "DoNotLock" false)
      (set `PlayerController.bShowMouseCursor` true _returnvalue)
      (`GameplayStatics.PlaySound2D` "/Game/AUDIO/SFX_Pickups/SC_Keycard.SC_Keycard" 0.75 0.6 0.06 null null)
      (`KismetSystemLibrary.Delay` 1.0)
      (`self.K2_DestroyActor`))))

(event `self.ReceiveBeginPlay`
  (bind _unlocked_ (`/Game/Blueprints/NewFunctionLibrary.has unlockable` "KNIFE"))
  (if _unlocked_
    (`self.K2_DestroyActor`)))

(fn `UserConstructionScript`)