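; Vending machine prop that breaks the first time it takes any damage and dispenses soda cans.
; Breaking swaps in a broken material, spawns smoke, sparks and sound, and sets the spotlight intensity.
; After a short delay, a delayed loop spawns a random number of BP_Sodacan actors at the Arrow, each with a sound.
; The construction script applies the intact Material; the projectile-tag and random-chance checks are disconnected.
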(event `self.ReceiveAnyDamage`
  (params (Damage :type "Float (single-precision)") (DamageType :type "DamageType Object Reference") (InstigatedBy :type "Controller Object Reference") (DamageCauser :type "Actor Object Reference"))
  (bind _arrow (`self.Arrow`))
  (bind _returnvalue (`SceneComponent.K2_GetComponentLocation` (`self.SpotLight`)))
  (`/Engine/EditorBlueprintResources/StandardMacros.DoOnce` false
    (:`Completed`
      (`PrimitiveComponent.SetMaterial` (`self.SM_VendMachine`) 1 (`self.broken material`))
      (`GameplayStatics.SpawnEmitterAtLocation` "/Game/StylizedNatureVol2/Effects/P_Stylized_Smoke.P_Stylized_Smoke" (+ _returnvalue (0.0 0.0 120.0)) (struct) (2.0 2.0 2.0))
      (`GameplayStatics.SpawnEmitterAtLocation` "/Game/kosm_fps_assets/Misc/Particles/P_Sparks1.P_Sparks1" _returnvalue)
      (`GameplayStatics.SpawnSoundAtLocation` "/Game/AUDIO/SFX_Damage/SC_Gibs_Robot.SC_Gibs_Robot" _returnvalue (struct) 1.0 1.0 0.0 null null)
      (`LightComponent.SetIntensity` (`self.SpotLight`) 2.0)
      (`KismetSystemLibrary.Delay` 1.0)
      (`/Game/MISSIONS/EP1/BP_MyMacroLibrary.For Loop With Delay` 0 (`KismetMathLibrary.RandomIntegerInRange` 0 5) 0.35
        (:`Loop Body`
          (`GameplayStatics.PlaySoundAtLocation` "/Game/AUDIO/SW_Grenade_launcher_reload1.SW_Grenade_launcher_reload1" (`SceneComponent.K2_GetComponentLocation` (`self.Arrow`)) (struct) 0.25 3.0 0.0 "/Game/kosm_fps_assets/Misc/SoundFX/SoundAttenuationLow.SoundAttenuationLow" null null)
          (`|SpawnActorFromClass` "/Game/MISSIONS/EP4/Blueprints/BP_Sodacan.BP_Sodacan_C" (`KismetMathLibrary.MakeTransform` (`SceneComponent.K2_GetComponentLocation` _arrow) (`SceneComponent.K2_GetComponentRotation` _arrow) (0.65 0.65 0.65)) "Undefined" "OverrideRootScale" null null))))))

(fn `UserConstructionScript`
  (`PrimitiveComponent.SetMaterial` (`self.SM_VendMachine`) 1 (`self.material`)))