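; Stain decal actor placed in the EP4 mission, with its look configurable per instance.
; The construction script creates a dynamic material instance on the Decal component and pushes the actor's variables into it, setting color, frame, emissive, roughness, specular and strength.
; It has no runtime logic, as the event graph holds only disabled default events.
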(fn `UserConstructionScript`
  (bind _returnvalue (`DecalComponent.CreateDynamicMaterialInstance` (`self.Decal`)))
  (`MaterialInstanceDynamic.SetVectorParameterValue` _returnvalue "Color" (`self.Color`))
  (`MaterialInstanceDynamic.SetScalarParameterValue` _returnvalue "Frame" (`self.Frame`))
  (`MaterialInstanceDynamic.SetScalarParameterValue` _returnvalue "Emissive" (`self.Emissive`))
  (`MaterialInstanceDynamic.SetScalarParameterValue` _returnvalue "RGH" (`self.Roughness`))
  (`MaterialInstanceDynamic.SetScalarParameterValue` _returnvalue "SPEC" (`self.Specular`))
  (`MaterialInstanceDynamic.SetScalarParameterValue` _returnvalue "Strength" (`self.Strength`)))