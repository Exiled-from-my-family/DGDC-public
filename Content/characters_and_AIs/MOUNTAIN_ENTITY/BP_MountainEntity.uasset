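; BP_MountainEntity is a mountain entity actor built from three skeletal meshes, with a material-driven appearance effect.
; The Appear event plays a timeline that lerps the Appearance scalar on all three meshes, creating new dynamic material instances on every update.
; The construction script presets that parameter on two of the meshes, leaving SKMountain untouched.
; Nothing here calls Appear, and a delayed timeline start is left disconnected.
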(event `Appear`
  (bind (_direction _appear) (`Timeline|Timeline_0` :!via `PlayFromStart`)
    (:`Update`
      (bind _returnvalue (`PrimitiveComponent.CreateDynamicMaterialInstance` (`self.SK_Mountain`) 0 "/Game/characters_and_AIs/MOUNTAIN_ENTITY/M_MountainEntity_Inst1.M_MountainEntity_Inst1" "None"))
      (bind _returnvalue_2 (`KismetMathLibrary.Lerp` 2.0 0.75 _appear))
      (`MaterialInstanceDynamic.SetScalarParameterValue` _returnvalue "Appearance" _returnvalue_2)
      (bind _returnvalue_3 (`PrimitiveComponent.CreateDynamicMaterialInstance` (`self.SkeletalMesh`) 0 "/Game/characters_and_AIs/MOUNTAIN_ENTITY/M_MountainEntity_Inst1.M_MountainEntity_Inst1" "None"))
      (`MaterialInstanceDynamic.SetScalarParameterValue` _returnvalue_3 "Appearance" _returnvalue_2)
      (bind _returnvalue_4 (`PrimitiveComponent.CreateDynamicMaterialInstance` (`self.SkeletalMesh1`) 0 "/Game/characters_and_AIs/MOUNTAIN_ENTITY/M_MountainEntity_Inst1.M_MountainEntity_Inst1" "None"))
      (`MaterialInstanceDynamic.SetScalarParameterValue` _returnvalue_4 "Appearance" _returnvalue_2))))

(event `self.ReceiveBeginPlay`)

(fn `UserConstructionScript`
  (bind _returnvalue (`PrimitiveComponent.CreateDynamicMaterialInstance` (`self.SkeletalMesh`) 0 "/Game/characters_and_AIs/MOUNTAIN_ENTITY/M_MountainEntity_Inst1.M_MountainEntity_Inst1" "None"))
  (`MaterialInstanceDynamic.SetScalarParameterValue` _returnvalue "Appearance" 0.5)
  (bind _returnvalue_2 (`PrimitiveComponent.CreateDynamicMaterialInstance` (`self.SkeletalMesh1`) 0 "/Game/characters_and_AIs/MOUNTAIN_ENTITY/M_MountainEntity_Inst1.M_MountainEntity_Inst1" "None"))
  (`MaterialInstanceDynamic.SetScalarParameterValue` _returnvalue_2 "Appearance" 0.5))