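; Tutorial point actor with a bobbing billboard that lets the player open a tutorial widget by pressing Interact nearby.
; Box overlap with the player character shows a prompt, opens an input gate and plays a timeline brightening the ring and light, reversed on exit.
; Interact pauses the game and shows the widget with mouse cursor.
; Pressing again or leaving removes it and restores game input, without unpausing here.
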(event `self.ReceiveBeginPlay`
  (bind (_direction _newtrack_0) (`Timeline|Billboard float` :!via `PlayFromStart`)
    (:`Update`
      (`SceneComponent.K2_SetRelativeLocation` (`self.Billboard`) (`KismetMathLibrary.VLerp` (0.0 0.0 200.0) (0.0 0.0 190.0) _newtrack_0) false false))))

(event `InputAction|Interact` :consume false
  (params (Key :type "Key Structure"))
  (bind _returnvalue (`GameplayStatics.GetPlayerController` 0))
  (bind _returnvalue_2 (`GameplayStatics.GetPlayerController` 0))
  (:`Pressed`
    (`/Engine/EditorBlueprintResources/StandardMacros.Gate` true :!label _label
      (:`Exit`
        (`/Engine/EditorBlueprintResources/StandardMacros.DoOnce` false :!label _label_2
          (:`Completed`
            (if (and (`self.IsNear?`) (not (`self.active`)))
              (set `self.active` true)
              (`GameplayStatics.SetGamePaused` true)
              (`Widget.RemoveFromParent` (`self.Text`)) ; removes "press E" text before showing tutorial widget
              (bind _returnvalue_3 (`|CreateWidget` (`self.Tutorial`) _returnvalue))
              (`UserWidget.AddToViewport` _returnvalue_3 0)
              (`WidgetBlueprintLibrary.SetInputMode_GameAndUIEx` _returnvalue _returnvalue_3 "DoNotLock" false)
              (set `PlayerController.bShowMouseCursor` true _returnvalue)
              (`GameplayStatics.PlaySound2D` "/Game/AUDIO/SFX_Pickups/SC_Keycard.SC_Keycard" 0.75 0.6 0.06 null null)
              (else
                (`WidgetBlueprintLibrary.SetInputMode_GameOnly` _returnvalue_2 :!label _label_3)
                (set `self.active` false)
                (set `PlayerController.bShowMouseCursor` false _returnvalue_2)
                (`/Engine/EditorBlueprintResources/StandardMacros.IsValid` _returnvalue_3
                  (:`Is Valid`
                    (`Widget.RemoveFromParent` _returnvalue_3))
                  (:`Is Not Valid`
                    _))))
            (`KismetSystemLibrary.Delay` 0.1)
            (goto _label_2 :!via `Reset`)))))))

(event `self.Box.OnComponentBeginOverlap`
  (params (OverlappedComponent :type "PrimitiveComponent Object Reference") (OtherActor :type "Actor Object Reference") (OtherComp :type "PrimitiveComponent Object Reference") (OtherBodyIndex :type Integer) (bFromSweep :type Boolean) (SweepResult :type "HitResult Structure (by ref)"))
  (cast `/Game/Blueprints/CHARACTERS/fpsMovementCharacter_light_1_vq3` OtherActor)
  (`self.Player steps in`)
  (set `self.IsNear?` true)
  (`/Game/Blueprints/NewFunctionLibrary.clean all message widgets`)
  (`KismetSystemLibrary.Delay` 0.01)
  (bind _returnvalue (`|CreateWidget` "/Game/Blueprints/UI/UI_Pickups/UI_GenericMessage.UI_GenericMessage_C" (`GameplayStatics.GetPlayerController` 0)))
  (bind _output_get (set `self.Text` _returnvalue))
  (set `/Game/Blueprints/UI/UI_Pickups/UI_GenericMessage.Message` "press 'E' to read the tutorial" _output_get)
  (set `/Game/Blueprints/UI/UI_Pickups/UI_GenericMessage.Duration` 5.0 _output_get)
  (`UserWidget.AddToViewport` _output_get 0)
  (goto _label :!via `Open`))

(event `self.Box.OnComponentEndOverlap`
  (params (OverlappedComponent :type "PrimitiveComponent Object Reference") (OtherActor :type "Actor Object Reference") (OtherComp :type "PrimitiveComponent Object Reference") (OtherBodyIndex :type Integer))
  (cast `/Game/Blueprints/CHARACTERS/fpsMovementCharacter_light_1_vq3` OtherActor)
  (`|ExecutionSequence`
    (:`then_0`
      (goto _label :!via `Close`))
    (:`then_1`
      (goto _label_3))
    (:`then_2`
      (`KismetSystemLibrary.Delay` 0.2)
      (`Widget.RemoveFromParent` (`self.Text`)))
    (:`then_3`
      (`self.Player steps out`))))

(event `Player steps in`
  (bind (_direction _radius_intensity _light_intensity) (`Timeline|Player in ring` :!via `PlayFromStart` :!label _label_4)
    (:`Update`
      (`MeshComponent.SetScalarParameterValueOnMaterials` (`self.Radius`) "Emissive" _radius_intensity)
      (`LightComponent.SetIntensity` (`self.PointLight`) _light_intensity))))

(event `Player steps out`
  (goto _label_4 :!via `Reverse`))

(fn `UserConstructionScript`
  (bind _radius (`self.Radius`))
  (`PrimitiveComponent.SetMaterial` _radius 0 "/Game/Blueprints/PICKUPS/M_ControlPointRadius_Inst1.M_ControlPointRadius_Inst1")
  (`MeshComponent.SetScalarParameterValueOnMaterials` _radius "Emissive" 6.0))