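; BP_laserSights is a laser sight that keeps a particle beam aimed at the player.
; Every tick it line-traces on Visibility from its location to the player's capsule, ignoring all EP3_robot_big actors, which it gathers anew each frame.
; The PSLaser5 beam target snaps to the hit point when blocked, otherwise to the capsule.
; A node setting the beam source is present but never executes.
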(event `self.ReceiveBeginPlay`)

(event `self.ReceiveTick`
  (params (DeltaSeconds :type "Float (single-precision)"))
  (bind _returnvalue (`SceneComponent.K2_GetComponentLocation` (`Character.CapsuleComponent` (`/Game/Blueprints/NewFunctionLibrary.get player PURE`))))
  (bind _outactors (`GameplayStatics.GetAllActorsOfClass` "/Game/MISSIONS/EP3/Characters/EP3_robot_big.EP3_robot_big_C"))
  (bind (_outhit _returnvalue_2) (`KismetSystemLibrary.LineTraceSingle` (`self.K2_GetActorLocation`) _returnvalue "TraceTypeQuery1" false _outactors))
  (if _returnvalue_2
    (`ParticleSystemComponent.SetBeamTargetPoint` (`self.PS_Laser5`) 0 (`.Location` (`GameplayStatics.BreakHitResult` _outhit)) 0)
    (else
      (`ParticleSystemComponent.SetBeamTargetPoint` (`self.PS_Laser5`) 0 _returnvalue 0))))

(fn `UserConstructionScript`)