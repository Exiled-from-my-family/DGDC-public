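; Demo save/load terminal with saving and loading disabled; it only gives proximity feedback and a refusal sound.
; When the player character enters the box, it fades in a loading loop, switches on the terminal material's Time parameter and shows a disabled-prompt widget.
; The overlap also opens a Gate for Interact, which plays a negative UI sound throttled by DoOnce and Delay.
; Leaving closes the gate, resets the material and fades out the loop.
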(event `self.ReceiveBeginPlay`
  (`AudioComponent.AdjustVolume` (`self.LoadingNumbers_03_Loop`) 0.0 0.0 "Linear"))

(event `InputAction|Interact` :consume false
  (params (Key :type "Key Structure"))
  (:`Pressed`
    (`/Engine/EditorBlueprintResources/StandardMacros.Gate` true :!label _label
      (:`Exit`
        (`/Engine/EditorBlueprintResources/StandardMacros.DoOnce` false :!label _label_2
          (:`Completed`
            (`GameplayStatics.PlaySound2D` "/Game/AUDIO/SFX_UI/SW_UI_Negative_2.SW_UI_Negative_2" 1.0 1.0 0.0 null null)
            (`KismetSystemLibrary.Delay` 0.1)
            (goto _label_2 :!via `Reset`)))))))

(event `self.Box.OnComponentBeginOverlap`
  (params (OverlappedComponent :type "PrimitiveComponent Object Reference") (OtherActor :type "Actor Object Reference") (OtherComp :type "PrimitiveComponent Object Reference") (OtherBodyIndex :type Integer) (bFromSweep :type Boolean) (SweepResult :type "HitResult Structure (by ref)"))
  (cast `/Game/Blueprints/CHARACTERS/fpsMovementCharacter_light_1_vq3` OtherActor)
  (set `self.IsNear?` true)
  (`AudioComponent.FadeIn` (`self.LoadingNumbers_03_Loop`) 0.2 0.2 0.0 "Linear")
  (`/Game/Blueprints/NewFunctionLibrary.clean all message widgets`)
  (`KismetSystemLibrary.Delay` 0.01)
  (bind _returnvalue (`|CreateWidget` "/Game/Blueprints/UI/UI_Pickups/UI_GenericMessage.UI_GenericMessage_C" (`GameplayStatics.GetPlayerController` 0)))
  (set `/Game/Blueprints/UI/UI_Pickups/UI_GenericMessage.Message` "press 'E' to save | load  \n(disabled)" _returnvalue)
  (`MeshComponent.SetScalarParameterValueOnMaterials` (`self.SM_terminal`) "Time" 1.0)
  (`UserWidget.AddToViewport` _returnvalue 0)
  (goto _label :!via `Open`))

(event `self.Box.OnComponentEndOverlap`
  (params (OverlappedComponent :type "PrimitiveComponent Object Reference") (OtherActor :type "Actor Object Reference") (OtherComp :type "PrimitiveComponent Object Reference") (OtherBodyIndex :type Integer))
  (cast `/Game/Blueprints/CHARACTERS/fpsMovementCharacter_light_1_vq3` OtherActor)
  (`|ExecutionSequence`
    (:`then_0`
      (goto _label :!via `Close`))
    (:`then_1`
      (`MeshComponent.SetScalarParameterValueOnMaterials` (`self.SM_terminal`) "Time" 0.0))
    (:`then_2`
      (`AudioComponent.FadeOut` (`self.LoadingNumbers_03_Loop`) 0.2 0.0 "Linear"))))

(fn `UserConstructionScript`
  (`MeshComponent.SetScalarParameterValueOnMaterials` (`self.SM_terminal`) "Time" 0.0))