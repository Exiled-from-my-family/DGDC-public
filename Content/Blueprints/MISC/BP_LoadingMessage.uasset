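; BP_LoadingMessage presents a level's loading screen when play begins, after loading the campaign difficulty.
; It disables player input and shooting tick, then shows UI_LoadingScreen with map text over a looping sound for LoadingTime.
; Afterwards it removes the screen, fades the camera in, starts music, restores the player, removes bot blockers and calls loading complete.
; The short-delay branch is unreachable because its condition is hardcoded true.
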(event `self.ReceiveBeginPlay`
  (`|ExecutionSequence`
    (:`then_0`
      (`/Game/Blueprints/NewFunctionLibrary.Load Difficulty Lvl Campaign`))
    (:`then_1`
      ;[1 1 1] Loading screen macro
      (bind _player (`/Game/Blueprints/NewFunctionLibrary.get player`))
      (`self.DisableInput` _player null)
      (set `/Game/Blueprints/CHARACTERS/fpsMovementCharacter_light_1_vq3.TICK SHOOTING` false _player)
      (bind _returnvalue (`GameplayStatics.SpawnSound2D` "/Game/AUDIO/SFX_UI/SW_Loading_Loop.SW_Loading_Loop" 0.1 1.0 0.0 null))
      (set `self.SFX` _returnvalue)
      (bind _returnvalue_2 (`|CreateWidget` "/Game/Blueprints/UI/UI_LoadingScreen.UI_LoadingScreen_C"))
      (set `/Game/Blueprints/UI/UI_LoadingScreen.LoadText` (`self.Text 1`) _returnvalue_2)
      (set `/Game/Blueprints/UI/UI_LoadingScreen.LoadText_2` (`self.Map name`) _returnvalue_2)
      (`UserWidget.AddToViewport` _returnvalue_2 12)
      (if true
        (`KismetSystemLibrary.Delay` (`self.Loading Time`))
        (else
          (`KismetSystemLibrary.Delay` 0.2)))
      (`AudioComponent.Stop` (`self.SFX`))
      (`Widget.RemoveFromParent` _returnvalue_2)
      (`PlayerCameraManager.StartCameraFade` :`self` (`GameplayStatics.GetPlayerCameraManager` 0) :`FromAlpha` 1.0 :`Duration` 1.0 :`bShouldFadeAudio` true)
      (`GameplayStatics.SpawnSound2D` (`self.Music`) 1.0 1.0 0.0 null)
      (bind _player_2 (`/Game/Blueprints/NewFunctionLibrary.get player`))
      (`self.EnableInput` _player_2 null)
      (`/Game/Blueprints/NewFunctionLibrary.remove bot blockers`)
      (`self.Loading complete`)
      (set `/Game/Blueprints/CHARACTERS/fpsMovementCharacter_light_1_vq3.TICK SHOOTING` true _player_2))))

(fn `UserConstructionScript`)