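; BP_ItemCounter is a trigger actor that tallies collectible items and shows a UI_ItemCounter widget when the player character overlaps its box.
; It counts all perma armor, website pickup and secret message actors, plus valid entries in ErroneouslyCountThese, storing the sum as both ItemsLeft and TotalItems.
; It clears message widgets before showing the counter, and a DoOnce blocks retriggering until the widget's duration elapses.
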(event `self.Box.OnComponentBeginOverlap`
  (params (OverlappedComponent :type "PrimitiveComponent Object Reference") (OtherActor :type "Actor Object Reference") (OtherComp :type "PrimitiveComponent Object Reference") (OtherBodyIndex :type Integer) (bFromSweep :type Boolean) (SweepResult :type "HitResult Structure (by ref)"))
  (cast `/Game/Blueprints/CHARACTERS/fpsMovementCharacter_light_1_vq3` OtherActor)
  (`/Engine/EditorBlueprintResources/StandardMacros.DoOnce` false :!label _label
    (:`Completed`
      (bind _outactors (`GameplayStatics.GetAllActorsOfClass` "/Game/Blueprints/PICKUPS/BP_Perma_Armor.BP_Perma_Armor_C"))
      (bind _outactors_2 (`GameplayStatics.GetAllActorsOfClass` "/Game/Blueprints/PICKUPS/BP_Website_Pickup.BP_Website_Pickup_C"))
      (bind _outactors_3 (`GameplayStatics.GetAllActorsOfClass` "/Game/Blueprints/MISC/BP_SecretMessage.BP_SecretMessage_C"))
      (bind _output_get (set `self.erroneous count` 0))
      (for _array_element (`self.erroneously count these`)
        (`/Engine/EditorBlueprintResources/StandardMacros.IsValid` _array_element
          (:`Is Valid`
            (`/Engine/EditorBlueprintResources/StandardMacros.IncrementInt` _output_get))))
      (bind _returnvalue (+ (`self.erroneous count`) (`KismetArrayLibrary.Array_Length` _outactors_2) (`KismetArrayLibrary.Array_Length` _outactors_3) (`KismetArrayLibrary.Array_Length` _outactors)))
      (set `self.Items left` _returnvalue)
      (set `self.Total items` _returnvalue)
      (`/Game/Blueprints/NewFunctionLibrary.clean all message widgets`)
      (`KismetSystemLibrary.Delay` 0.1)
      (bind _returnvalue_2 (`|CreateWidget` "/Game/Blueprints/UI/UI_Pickups/UI_ItemCounter.UI_ItemCounter_C"))
      (`UserWidget.AddToViewport` _returnvalue_2 0)
      (`KismetSystemLibrary.Delay` (`/Game/Blueprints/UI/UI_Pickups/UI_ItemCounter.Duration` _returnvalue_2))
      (goto _label :!via `Reset`))))

(fn `UserConstructionScript`)