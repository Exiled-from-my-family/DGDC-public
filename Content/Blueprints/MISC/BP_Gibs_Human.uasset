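; BP_Gibs_Human is a human gore effect actor made of five gib components, a radial force and a blood decal.
; On BeginPlay it randomizes its yaw, fires a radial impulse to scatter the gibs and applies one of eight random bloodstain decal materials.
; If DestroyIn5Seconds is set, it toggles gib visibility after five seconds and destroys the whole actor 25 seconds later, despite the flag's name.
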(event `self.ReceiveBeginPlay`
  (`self.K2_SetActorRotation` (`KismetMathLibrary.MakeRotator` 0.0 0.0 (`KismetMathLibrary.RandomFloatInRange` 0.0 180.0)))
  (`RadialForceComponent.FireImpulse` (`self.RadialForce`))
  (`DecalComponent.SetDecalMaterial` (`self.Decal`) (select `int` (`KismetMathLibrary.RandomIntegerInRange` 0 7) :`0` "/Game/kosm_fps_assets/Misc/Materials/D_BloodStain_Inst.D_BloodStain_Inst" :`1` "/Game/kosm_fps_assets/Misc/Materials/D_BloodStain_Inst1.D_BloodStain_Inst1" :`2` "/Game/kosm_fps_assets/Misc/Materials/D_BloodStain_Inst2.D_BloodStain_Inst2" :`3` "/Game/kosm_fps_assets/Misc/Materials/D_BloodStain_Inst3.D_BloodStain_Inst3" :`4` "/Game/kosm_fps_assets/Misc/Materials/D_BloodStain_Inst4.D_BloodStain_Inst4" :`5` "/Game/kosm_fps_assets/Misc/Materials/D_BloodStain_Inst5.D_BloodStain_Inst5" :`6` "/Game/kosm_fps_assets/Misc/Materials/D_BloodStain_Inst6.D_BloodStain_Inst6" :`7` "/Game/kosm_fps_assets/Misc/Materials/D_BloodStain_Inst7.D_BloodStain_Inst7" :!type "MaterialInterface Object Reference"))
  (if (`self.destroy in 5 seconds`)
    (`KismetSystemLibrary.Delay` 5.0)
    (`SceneComponent.ToggleVisibility` (`self.Gib2`) true)
    (`SceneComponent.ToggleVisibility` (`self.Gib1`) true)
    (`SceneComponent.ToggleVisibility` (`self.Gib4`) true)
    (`SceneComponent.ToggleVisibility` (`self.Gib5`) true)
    (`SceneComponent.ToggleVisibility` (`self.Gib3`) true)
    (`KismetSystemLibrary.Delay` 25.0)
    (`self.K2_DestroyActor`)))

(fn `UserConstructionScript`)