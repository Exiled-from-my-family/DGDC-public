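; BP_GenericMessage is a trigger actor that shows an on-screen message when the player character enters its Box.
; On overlap by fpsMovementCharacter_light_1_vq3, it calls CleanAllMessageWidgets, then creates a UI_GenericMessage_alt widget with its Message and Duration and adds it to the viewport.
; A DoOnce gate blocks repeat messages and resets one second after the character leaves the Box.
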(event `self.Box.OnComponentBeginOverlap`
  (params (OverlappedComponent :type "PrimitiveComponent Object Reference") (OtherActor :type "Actor Object Reference") (OtherComp :type "PrimitiveComponent Object Reference") (OtherBodyIndex :type Integer) (bFromSweep :type Boolean) (SweepResult :type "HitResult Structure (by ref)"))
  (cast `/Game/Blueprints/CHARACTERS/fpsMovementCharacter_light_1_vq3` OtherActor)
  (`/Engine/EditorBlueprintResources/StandardMacros.DoOnce` false :!label _label
    (:`Completed`
      (`/Game/Blueprints/NewFunctionLibrary.clean all message widgets`)
      (bind _returnvalue (`|CreateWidget` "/Game/Blueprints/UI/UI_Pickups/UI_GenericMessage_alt.UI_GenericMessage_alt_C"))
      (set `/Game/Blueprints/UI/UI_Pickups/UI_GenericMessage_alt.Message` (`self.Message`) _returnvalue)
      (set `/Game/Blueprints/UI/UI_Pickups/UI_GenericMessage_alt.Duration` (`self.Duration`) _returnvalue)
      (`UserWidget.AddToViewport` _returnvalue 0))))

(event `self.Box.OnComponentEndOverlap`
  (params (OverlappedComponent :type "PrimitiveComponent Object Reference") (OtherActor :type "Actor Object Reference") (OtherComp :type "PrimitiveComponent Object Reference") (OtherBodyIndex :type Integer))
  (cast `/Game/Blueprints/CHARACTERS/fpsMovementCharacter_light_1_vq3` OtherActor)
  (`KismetSystemLibrary.Delay` 1.0)
  (goto _label :!via `Reset`))

(fn `UserConstructionScript`)