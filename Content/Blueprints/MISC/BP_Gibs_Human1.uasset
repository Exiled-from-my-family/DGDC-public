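; BP_Gibs_Human1 is a short-lived human gib effect that scatters pieces and shows a decal.
; On BeginPlay it takes a random yaw, fires a radial force impulse and sets a random "Frame" parameter on the decal's dynamic material for variety.
; After a delay it toggles the gib components' visibility, then destroys the whole actor after a longer delay.
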(event `self.ReceiveBeginPlay`
  (`self.K2_SetActorRotation` (`KismetMathLibrary.MakeRotator` 0.0 0.0 (`KismetMathLibrary.RandomFloatInRange` 0.0 180.0)))
  (`RadialForceComponent.FireImpulse` (`self.RadialForce`))
  (bind _returnvalue (`DecalComponent.CreateDynamicMaterialInstance` (`self.Decal`)))
  (`MaterialInstanceDynamic.SetScalarParameterValue` _returnvalue "Frame" (`KismetMathLibrary.RandomFloatInRange` 1.0 8.0))
  (`KismetSystemLibrary.Delay` 5.0)
  (`SceneComponent.ToggleVisibility` (`self.Gib2`) true)
  (`SceneComponent.ToggleVisibility` (`self.Gib1`) true)
  (`SceneComponent.ToggleVisibility` (`self.Gib4`) true)
  (`SceneComponent.ToggleVisibility` (`self.Gib5`) true)
  (`SceneComponent.ToggleVisibility` (`self.Gib3`) true)
  (`KismetSystemLibrary.Delay` 25.0)
  (`self.K2_DestroyActor`))

(fn `UserConstructionScript`)