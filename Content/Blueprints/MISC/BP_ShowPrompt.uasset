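; Trigger-box actor that shows a persistent "Interact" keybind prompt with its Action while the player character overlaps it.
; Begin overlap clears other message widgets, then after a tiny delay creates the prompt with zero duration, unless already on screen.
; It also opens a Tick gate that removes the prompt once no player overlaps, then closes.
; End overlap removes the prompt only if the player has nonzero velocity.
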(event `self.ReceiveBeginPlay`)

(event `self.ReceiveTick`
  (params (DeltaSeconds :type "Float (single-precision)"))
  (bind _prompt (`self.prompt`))
  (`/Engine/EditorBlueprintResources/StandardMacros.Gate` true :!label _label
    (:`Exit`
      (if (not (`KismetMathLibrary.Conv_IntToBool` (`KismetArrayLibrary.Array_Length` (`PrimitiveComponent.GetOverlappingActors` (`self.Box`) "/Game/Blueprints/CHARACTERS/fpsMovementCharacter_light_1_vq3.fpsMovementCharacter_light_1_vq3_C"))))
        (`/Engine/EditorBlueprintResources/StandardMacros.IsValid` _prompt
          (:`Is Valid`
            (`Widget.RemoveFromParent` _prompt)
            (goto _label :!via `Close`))
          (:`Is Not Valid`
            (`/Game/Blueprints/NewFunctionLibrary.clean all message widgets`)
            (goto _label :!via `Close`)))))))

(event `self.Box.OnComponentBeginOverlap`
  (params (OverlappedComponent :type "PrimitiveComponent Object Reference") (OtherActor :type "Actor Object Reference") (OtherComp :type "PrimitiveComponent Object Reference") (OtherBodyIndex :type Integer) (bFromSweep :type Boolean) (SweepResult :type "HitResult Structure (by ref)"))
  (`|ExecutionSequence`
    (:`then_0`
      (cast `/Game/Blueprints/CHARACTERS/fpsMovementCharacter_light_1_vq3` OtherActor)
      (set `self.IsNear?` true)
      (`/Game/Blueprints/NewFunctionLibrary.clean all message widgets`)
      (`KismetSystemLibrary.Delay` 0.01)
      (`/Engine/EditorBlueprintResources/StandardMacros.IsValid` (stale `self.Box.OnComponentBeginOverlap` _output_get)
        (:`Is Valid`
          (if (not (`Widget.IsInViewport` (stale `self.Box.OnComponentBeginOverlap` _output_get)))
            (bind _returnvalue (`|CreateWidget` "/Game/Blueprints/UI/UI_PauseTutorials/UI_GenericMessage_Keybind.UI_GenericMessage_Keybind_C" (`GameplayStatics.GetPlayerController` 0) "Interact" "" 0.0 :!label _label_2))
            (bind _output_get (set `self.prompt` _returnvalue))
            (set `/Game/Blueprints/UI/UI_PauseTutorials/UI_GenericMessage_Keybind.InputAction` "Interact" _output_get)
            (set `/Game/Blueprints/UI/UI_PauseTutorials/UI_GenericMessage_Keybind.action` (`self.Action`) _output_get)
            (set `/Game/Blueprints/UI/UI_PauseTutorials/UI_GenericMessage_Keybind.Duration` 0.0 _output_get :!pinned true) ; THEY COMPLAINED THAT IT DISAPEARED AT ALL
            (`UserWidget.AddToViewport` _output_get -1)))
        (:`Is Not Valid`
          (goto _label_2))))
    (:`then_1`
      (goto _label :!via `Open`))))

(event `self.Box.OnComponentEndOverlap`
  (params (OverlappedComponent :type "PrimitiveComponent Object Reference") (OtherActor :type "Actor Object Reference") (OtherComp :type "PrimitiveComponent Object Reference") (OtherBodyIndex :type Integer))
  (bind _asfps_movement_character_light_1_vq_3 (cast `/Game/Blueprints/CHARACTERS/fpsMovementCharacter_light_1_vq3` OtherActor))
  (if (not (== (`self.GetVelocity` _asfps_movement_character_light_1_vq_3) (0.0 0.0 0.0)))
    (`/Engine/EditorBlueprintResources/StandardMacros.IsValid` (stale `self.Box.OnComponentBeginOverlap` _output_get)
      (:`Is Valid`
        (`Widget.RemoveFromParent` (stale `self.Box.OnComponentBeginOverlap` _output_get))))))

(fn `UserConstructionScript`)