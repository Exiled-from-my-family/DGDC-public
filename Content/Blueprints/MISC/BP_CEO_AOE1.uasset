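; Expanding blastwave AOE, apparently for the CEO mecha boss, that shakes the camera on spawn and destroys itself when done.
; A timeline scales the mesh outward, and its overlap with a living player triggers a radial fan of line traces ignoring the mecha to check line of sight.
; A trace hit on the player once applies damage and camera shake, launches and stuns them airborne, then pulls them horizontally toward the blast origin.
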(event `self.StaticMesh.OnComponentBeginOverlap`
  (params (OverlappedComponent :type "PrimitiveComponent Object Reference") (OtherActor :type "Actor Object Reference") (OtherComp :type "PrimitiveComponent Object Reference") (OtherBodyIndex :type Integer) (bFromSweep :type Boolean) (SweepResult :type "HitResult Structure (by ref)"))
  (bind _player (`/Game/Blueprints/NewFunctionLibrary.get player PURE`))
  (bind _newvar_0 (`self.NewVar_0`))
  (bind _returnvalue (+ (`self.K2_GetActorLocation`) (0.0 0.0 50.0)))
  (bind _asfps_movement_character_light_1_vq_3 (cast `/Game/Blueprints/CHARACTERS/fpsMovementCharacter_light_1_vq3` OtherActor))
  (if (not (`/Game/Blueprints/CHARACTERS/fpsMovementCharacter_light_1_vq3.IsDead?` _asfps_movement_character_light_1_vq_3))
    (bind _outactors (`GameplayStatics.GetAllActorsOfClass` "/Game/MISSIONS/EP6/Characters/EP6_CEOMECHA_v2.EP6_CEOMECHA_v2_C"))
    ;[1 1 1] Radial line trace to check if something obstructs LOS between blastwave and player
    (for _index (range (+ _newvar_0 1))
      (bind (_outhit _returnvalue_2) (`KismetSystemLibrary.LineTraceSingle` _returnvalue (+ _returnvalue (* (`KismetMathLibrary.GreaterGreater_VectorRotator` (`self.GetActorForwardVector`) (`KismetMathLibrary.MakeRotator` 0.0 0.0 (* _index (/ 360.0 (`KismetMathLibrary.Conv_IntToDouble` (+ _newvar_0 1)))))) 8000.0)) "TraceTypeQuery1" true _outactors "None" true (struct :`R` 1.0 :`A` 1.0) (struct :`G` 1.0 :`A` 1.0) 1.0))
      (if _returnvalue_2
        (bind _asfps_movement_character_light_1_vq_3_2 (cast `/Game/Blueprints/CHARACTERS/fpsMovementCharacter_light_1_vq3` (`.HitActor` (`GameplayStatics.BreakHitResult` _outhit))))
        (`/Engine/EditorBlueprintResources/StandardMacros.DoOnce` false
          (:`Completed`
            (`GameplayStatics.ApplyDamage` _asfps_movement_character_light_1_vq_3_2 20.0)
            (`PlayerCameraManager.PlayCameraShake` :`self` (`GameplayStatics.GetPlayerCameraManager` 0) :`ShakeClass` "/Game/Blueprints/SHAKES/BP_CameraShake_Explosion.BP_CameraShake_Explosion_C" :`Scale` 2.0)
            (`Character.LaunchCharacter` _player (0.0 0.0 4000.0) false true)
            (`/Game/Blueprints/CHARACTERS/fpsMovementCharacter_light_1_vq3.Stunned_InAir` _player 1.0)
            (`KismetSystemLibrary.Delay` 0.05)
            (`Character.LaunchCharacter` (`/Game/Blueprints/NewFunctionLibrary.get player PURE`) (* (`KismetMathLibrary.GetForwardVector` (`KismetMathLibrary.FindLookAtRotation` (`self.K2_GetActorLocation`) (`self.K2_GetActorLocation` (`/Game/Blueprints/NewFunctionLibrary.get player PURE`)))) -1000.0) true false)))))))

(event `self.ReceiveBeginPlay`
  (`GameplayStatics.PlayWorldCameraShake` "/Game/Blueprints/SHAKES/BP_CameraShake_Explosion.BP_CameraShake_Explosion_C" (`self.K2_GetActorLocation`) 500.0 2500.0 0.5)
  (bind (_direction _expand) (`Timeline|BlastRadius` :!via `PlayFromStart`)
    (:`Update`
      (`SceneComponent.SetRelativeScale3D` (`self.StaticMesh`) (`KismetMathLibrary.VLerp` (0.1 0.1 2.0) (6.0 6.0 2.0) _expand)))
    (:`Finished`
      (`self.K2_DestroyActor`))))

(fn `UserConstructionScript`)