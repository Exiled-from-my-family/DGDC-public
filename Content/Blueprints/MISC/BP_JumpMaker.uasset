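; BP_JumpMaker is a jump pad that launches Ep1_character actors that touch it.
; Each jump is two overriding launches: JumpHeight first, then, after a brief delay, JumpDistance along the Arrow's forward vector.
; The Box overlap event triggers the jump, then briefly hides the pad and disables its collision before restoring it.
; Tick also polls overlapping characters through a short Delay and applies the same launch sequence.
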(event `self.ReceiveTick`
  (params (DeltaSeconds :type "Float (single-precision)"))
  (`KismetSystemLibrary.Delay` 0.1)
  (for _array_element (`self.GetOverlappingActors` "/Game/MISSIONS/EP1/Characters/ep1_character.ep1_character_C")
    (bind _ascharacter (cast `Character` _array_element))
    (`/Engine/EditorBlueprintResources/StandardMacros.IsValid` _array_element
      (:`Is Valid`
        (`Character.LaunchCharacter` _ascharacter (`self.Jump height`) true true)
        (`KismetSystemLibrary.Delay` 0.05)
        (`/Engine/EditorBlueprintResources/StandardMacros.IsValid` _ascharacter
          (:`Is Valid`
            (`Character.LaunchCharacter` _ascharacter (* (`SceneComponent.GetForwardVector` (`self.Arrow`)) (`self.Jump distance`)) true true)))))))

(event `self.Box.OnComponentBeginOverlap`
  (params (OverlappedComponent :type "PrimitiveComponent Object Reference") (OtherActor :type "Actor Object Reference") (OtherComp :type "PrimitiveComponent Object Reference") (OtherBodyIndex :type Integer) (bFromSweep :type Boolean) (SweepResult :type "HitResult Structure (by ref)"))
  (bind _asep_1_character (cast `/Game/MISSIONS/EP1/Characters/ep1_character` OtherActor))
  (`Character.LaunchCharacter` _asep_1_character (`self.Jump height`) true true)
  (`KismetSystemLibrary.Delay` 0.05)
  (`/Engine/EditorBlueprintResources/StandardMacros.IsValid` _asep_1_character
    (:`Is Valid`
      (`Character.LaunchCharacter` _asep_1_character (* (`SceneComponent.GetForwardVector` (`self.Arrow`)) (`self.Jump distance`)) true true)
      (`self.SetActorHiddenInGame` true)
      (`self.SetActorEnableCollision` false)
      (`KismetSystemLibrary.Delay` 0.5)
      (`self.SetActorHiddenInGame` false)
      (`self.SetActorEnableCollision` true))))

(fn `UserConstructionScript`)