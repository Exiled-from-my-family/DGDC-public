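; BP_TutorialEditable is a placeable tutorial marker that shows an editable message popup when the player touches it.
; At BeginPlay it hides if the saved tutorial option is off, self-destructs if its Unlockable is owned, or else floats its billboard.
; The Box overlap fades ring and light through a timeline.
; The Sphere fires once, grants the Unlockable and opens W_PauseTutorialGeneric, whose close event re-enables jumping and destroys the actor.
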(event `self.ReceiveBeginPlay`
  (bind _returnvalue (`GameplayStatics.DoesSaveGameExist` "Misc"))
  (if _returnvalue
    (bind _returnvalue_2 (`GameplayStatics.LoadGameFromSlot` "Misc"))
    (bind _asbp_save_game_options (cast `/Game/MenuBuilderCarousel/Blueprints/BP_SaveGameOptions` _returnvalue_2)
      (:`then`
        (if (`/Game/MenuBuilderCarousel/Blueprints/BP_SaveGameOptions.MISC_tutorial` _asbp_save_game_options)
          (bind _unlocked_ (`/Game/Blueprints/NewFunctionLibrary.has unlockable` (`self.unlockable`) :!label _label))
          (if _unlocked_
            (`self.K2_DestroyActor`)
            (else
              (bind (_direction _newtrack_0) (`Timeline|Billboard float` :!via `PlayFromStart`)
                (:`Update`
                  (`SceneComponent.K2_SetRelativeLocation` (`self.Billboard`) (`KismetMathLibrary.VLerp` (0.0 0.0 200.0) (0.0 0.0 190.0) _newtrack_0) false false)))))
          (else
            (`self.HIDE Tutorial`))))
      (:`CastFailed`
        (goto _label)))
    (else
      (goto _label))))

(event `HIDE Tutorial`
  (`self.SetActorHiddenInGame` true)
  (`self.SetActorEnableCollision` false))

(event `self.Box.OnComponentBeginOverlap`
  (params (OverlappedComponent :type "PrimitiveComponent Object Reference") (OtherActor :type "Actor Object Reference") (OtherComp :type "PrimitiveComponent Object Reference") (OtherBodyIndex :type Integer) (bFromSweep :type Boolean) (SweepResult :type "HitResult Structure (by ref)"))
  (cast `/Game/Blueprints/CHARACTERS/fpsMovementCharacter_light_1_vq3` OtherActor)
  (`self.Player steps in`))

(event `SHOW Tutorial`
  (`self.SetActorHiddenInGame` false)
  (`self.SetActorEnableCollision` true))

(event `self.Box.OnComponentEndOverlap`
  (params (OverlappedComponent :type "PrimitiveComponent Object Reference") (OtherActor :type "Actor Object Reference") (OtherComp :type "PrimitiveComponent Object Reference") (OtherBodyIndex :type Integer))
  (cast `/Game/Blueprints/CHARACTERS/fpsMovementCharacter_light_1_vq3` OtherActor)
  (`self.Player steps out`))

(event `Player steps in`
  (bind (_direction _radius_intensity _light_intensity) (`Timeline|Player in ring` :!via `PlayFromStart` :!label _label_2)
    (:`Update`
      (`MeshComponent.SetScalarParameterValueOnMaterials` (`self.Radius`) "Emissive" _radius_intensity)
      (`LightComponent.SetIntensity` (`self.PointLight`) _light_intensity))))

(event `Player steps out`
  (goto _label_2 :!via `Reverse`))

(event `self.Sphere.OnComponentBeginOverlap`
  (params (OverlappedComponent :type "PrimitiveComponent Object Reference") (OtherActor :type "Actor Object Reference") (OtherComp :type "PrimitiveComponent Object Reference") (OtherBodyIndex :type Integer) (bFromSweep :type Boolean) (SweepResult :type "HitResult Structure (by ref)"))
  (cast `/Game/Blueprints/CHARACTERS/fpsMovementCharacter_light_1_vq3` OtherActor)
  (`/Engine/EditorBlueprintResources/StandardMacros.DoOnce` false
    (:`Completed`
      (`KismetSystemLibrary.Delay` 0.1)
      (`self.Tutorial`)
      (`self.SetActorHiddenInGame` true))))

(event `Tutorial`
  (`/Game/Blueprints/NewFunctionLibrary.add unlockable` (`self.unlockable`))
  (bind _returnvalue (`|CreateWidget` "/Game/Blueprints/UI/UI_PauseTutorials/W_PauseTutorialGeneric.W_PauseTutorialGeneric_C" (`GameplayStatics.GetPlayerController` 0) true (`self.delay b4 quitting is enabled`)))
  (set `/Game/Blueprints/UI/UI_PauseTutorials/W_PauseTutorialGeneric.Message` (`self.Tutorial Text`) _returnvalue)
  (`UserWidget.AddToViewport` _returnvalue 0)
  (`GameplayStatics.PlaySound2D` "/Game/AUDIO/SFX_Pickups/SC_Keycard.SC_Keycard" 0.75 0.6 0.06 null null)
  (add `/Game/Blueprints/UI/UI_PauseTutorials/W_PauseTutorialGeneric.Close Tutorial` _returnvalue (delegate `Add tutorial unlockable`)))

(event `Add tutorial unlockable`
  (`KismetSystemLibrary.Delay` 1.0)
  (bind _player (`/Game/Blueprints/NewFunctionLibrary.get player`)) ; player can jump again
  (set `/Game/Blueprints/CHARACTERS/fpsMovementCharacter_light_1_vq3.CanJump?` true _player)
  (`self.K2_DestroyActor`))

(fn `UserConstructionScript`
  (bind _radius (`self.Radius`))
  (`PrimitiveComponent.SetMaterial` _radius 0 "/Game/Blueprints/PICKUPS/M_ControlPointRadius_Inst1.M_ControlPointRadius_Inst1")
  (`MeshComponent.SetScalarParameterValueOnMaterials` _radius "Emissive" 6.0))