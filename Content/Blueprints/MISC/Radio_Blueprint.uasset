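; Radio actor that plays a static sound and shows a text label when something overlaps its sphere.
; Tick polls the Jebaited flag: false spawns the static cue at the actor's location, and true stops it.
; Two DoOnce nodes reset each other, so sound changes fire once per flag flip rather than every frame.
; Sphere begin and end overlap events toggle the TextRender's visibility, with no filter on the overlapping actor.
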(event `self.ReceiveTick`
  (params (DeltaSeconds :type "Float (single-precision)"))
  (if (`self.Jebaited`)
    (`/Engine/EditorBlueprintResources/StandardMacros.DoOnce` false :!label _label
      (:`Completed`
        (`AudioComponent.Stop` (stale _returnvalue))
        (goto _label_2 :!via `Reset`)))
    (else
      (`/Engine/EditorBlueprintResources/StandardMacros.DoOnce` false :!label _label_2
        (:`Completed`
          (bind _returnvalue (`GameplayStatics.SpawnSoundAtLocation` "/Game/AUDIO/static_Cue.static_Cue" (`self.K2_GetActorLocation`) (struct) 1.0 1.0 0.0 null null))
          (goto _label :!via `Reset`))))))

(event `self.ReceiveBeginPlay`)

(event `self.Sphere.OnComponentBeginOverlap`
  (params (OverlappedComponent :type "PrimitiveComponent Object Reference") (OtherActor :type "Actor Object Reference") (OtherComp :type "PrimitiveComponent Object Reference") (OtherBodyIndex :type Integer) (bFromSweep :type Boolean) (SweepResult :type "HitResult Structure (by ref)"))
  (`SceneComponent.SetVisibility` (`self.TextRender`) true false))

(event `self.Sphere.OnComponentEndOverlap`
  (params (OverlappedComponent :type "PrimitiveComponent Object Reference") (OtherActor :type "Actor Object Reference") (OtherComp :type "PrimitiveComponent Object Reference") (OtherBodyIndex :type Integer))
  (`SceneComponent.SetVisibility` (`self.TextRender`) false false))

(fn `UserConstructionScript`)