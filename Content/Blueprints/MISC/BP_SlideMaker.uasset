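; BP_SlideMaker is a trigger volume that makes the player's FPS movement character slide off the surface it covers.
; Entering its Capsule zeroes ground friction, braking friction and walkable floor angle on the character's movement component, and prints a debug message.
; Leaving waits briefly, restores hard-coded movement values, then resets the DoOnce gating entry.
; That gate precedes the character cast, so any overlapping actor can consume it.
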(event `self.Capsule.OnComponentBeginOverlap`
  (params (OverlappedComponent :type "PrimitiveComponent Object Reference") (OtherActor :type "Actor Object Reference") (OtherComp :type "PrimitiveComponent Object Reference") (OtherBodyIndex :type Integer) (bFromSweep :type Boolean) (SweepResult :type "HitResult Structure (by ref)"))
  (`/Engine/EditorBlueprintResources/StandardMacros.DoOnce` false :!label _label
    (:`Completed`
      (bind _asfps_movement_character_light_1_vq_3 (cast `/Game/Blueprints/CHARACTERS/fpsMovementCharacter_light_1_vq3` OtherActor))
      (bind _charactermovement (`Character.CharacterMovement` _asfps_movement_character_light_1_vq_3))
      (set `CharacterMovementComponent.GroundFriction` 0.0 _charactermovement)
      (set `CharacterMovementComponent.BrakingFrictionFactor` 0.0 _charactermovement)
      (`CharacterMovementComponent.SetWalkableFloorAngle` _charactermovement 0.0)
      (`KismetSystemLibrary.PrintString` "slide off this surface" true true (struct :`R` 1.0 :`B` 0.829491 :`A` 1.0) 1.0))))

(event `self.Capsule.OnComponentEndOverlap`
  (params (OverlappedComponent :type "PrimitiveComponent Object Reference") (OtherActor :type "Actor Object Reference") (OtherComp :type "PrimitiveComponent Object Reference") (OtherBodyIndex :type Integer))
  (`KismetSystemLibrary.Delay` 0.2)
  (bind _asfps_movement_character_light_1_vq_3 (cast `/Game/Blueprints/CHARACTERS/fpsMovementCharacter_light_1_vq3` OtherActor))
  (bind _charactermovement (`Character.CharacterMovement` _asfps_movement_character_light_1_vq_3))
  (set `CharacterMovementComponent.GroundFriction` 8.0 _charactermovement)
  (set `CharacterMovementComponent.BrakingFrictionFactor` 1.5 _charactermovement)
  (`CharacterMovementComponent.SetWalkableFloorAngle` _charactermovement 60.0)
  (goto _label :!via `Reset`))

(fn `UserConstructionScript`)