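; Save station terminal that lets the player open a save list tagged with the station's number.
; Tick polls a box overlap to toggle the keybind prompt, terminal material and looping sound, and gates the Interact input.
; Interacting opens the list widget and pauses the game; closing it restores input and unpauses, with DoOnce and Delay debouncing.
; The construction script derives the station number from its index among all placed stations.
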(event `self.ReceiveBeginPlay`
  (`AudioComponent.AdjustVolume` (`self.LoadingNumbers_03_Loop`) 0.0 0.0 "Linear")
  (`self.EnableInput` (`GameplayStatics.GetPlayerController` 0)))

(event `self.ReceiveTick`
  (params (DeltaSeconds :type "Float (single-precision)"))
  (`/Engine/EditorBlueprintResources/StandardMacros.IsValid` (`|GetArrayItem` (`PrimitiveComponent.GetOverlappingActors` (`self.Box`) "/Game/Blueprints/CHARACTERS/fpsMovementCharacter_light_1_vq3.fpsMovementCharacter_light_1_vq3_C"))
    (:`Is Valid`
      (`/Engine/EditorBlueprintResources/StandardMacros.DoOnce` false :!label _label
        (:`Completed`
          (set `self.IsNear?` true)
          (`AudioComponent.FadeIn` (`self.LoadingNumbers_03_Loop`) 0.2 0.2 0.0 "Linear")
          (bind _foundwidgets (`WidgetBlueprintLibrary.GetAllWidgetsOfClass` "/Game/Blueprints/UI/UI_Pickups/UI_ItemCounter.UI_ItemCounter_C"))
          (`Widget.RemoveFromParent` _foundwidgets)
          (bind _returnvalue (`|CreateWidget` "/Game/Blueprints/UI/UI_PauseTutorials/UI_GenericMessage_Keybind.UI_GenericMessage_Keybind_C" (`GameplayStatics.GetPlayerController` 0) "Interact" "" 0.0))
          (bind _output_get (set `self.prompt` _returnvalue))
          (set `/Game/Blueprints/UI/UI_PauseTutorials/UI_GenericMessage_Keybind.InputAction` "Interact" _output_get)
          (set `/Game/Blueprints/UI/UI_PauseTutorials/UI_GenericMessage_Keybind.action` "to access the Save Station" _output_get)
          (set `/Game/Blueprints/UI/UI_PauseTutorials/UI_GenericMessage_Keybind.Duration` 0.0 _output_get :!pinned true) ; THEY COMPLAINED THAT IT DISAPEARED AT ALL
          (`UserWidget.AddToViewport` _output_get -1)
          (`MeshComponent.SetScalarParameterValueOnMaterials` (`self.SM_terminal`) "Time" 1.0)
          (goto _label_2 :!via `Open`))))
    (:`Is Not Valid`
      (`|ExecutionSequence`
        (:`then_0`
          (`|ExecutionSequence`
            (:`then_0`
              (`/Engine/EditorBlueprintResources/StandardMacros.IsValid` _returnvalue
                (:`Is Valid`
                  (`Widget.RemoveFromParent` _returnvalue)
                  (goto _label_2 :!via `Close`))
                (:`Is Not Valid`
                  (goto _label_2 :!via `Close`))))
            (:`then_1`
              (`MeshComponent.SetScalarParameterValueOnMaterials` (`self.SM_terminal`) "Time" 0.0))
            (:`then_2`
              (`AudioComponent.FadeOut` (`self.LoadingNumbers_03_Loop`) 0.2 0.0 "Linear"))))
        (:`then_1`
          (goto _label :!via `Reset`))))))

(event `InputAction|Interact` :consume false
  (params (Key :type "Key Structure"))
  (:`Pressed`
    (`/Engine/EditorBlueprintResources/StandardMacros.Gate` true :!label _label_2
      (:`Exit`
        (`/Engine/EditorBlueprintResources/StandardMacros.DoOnce` false :!label _label_3
          (:`Completed`
            (if (and (`self.IsNear?`) (not (`self.active`)))
              (set `self.active` true)
              (bind _returnvalue (`|CreateWidget` "/Game/MenuBuilderCarousel/UMG/savelist_for_terminal.savelist_for_terminal_C" (`GameplayStatics.GetPlayerController` 0) (`self.station`)))
              (add `/Game/MenuBuilderCarousel/UMG/savelist_for_terminal.close savelist` _returnvalue (delegate `Close savelist`))
              (`UserWidget.AddToViewport` _returnvalue 0)
              (`WidgetBlueprintLibrary.SetInputMode_UIOnlyEx` (`GameplayStatics.GetPlayerController` 0) _returnvalue)
              (`GameplayStatics.PlaySound2D` "/Game/AUDIO/SFX_Pickups/SC_Keycard.SC_Keycard" 0.75 0.6 0.06 null null)
              (set `PlayerController.bShowMouseCursor` true (`GameplayStatics.GetPlayerController` 0))
              (`|ExecutionSequence`
                (:`then_0`
                  (`GameplayStatics.SetGamePaused` true)
                  (`KismetSystemLibrary.Delay` 0.1 :!label _label_4)
                  (goto _label_3 :!via `Reset`))))))))))

(event `Close savelist`
  (`WidgetBlueprintLibrary.SetInputMode_GameOnly` (`GameplayStatics.GetPlayerController` 0))
  (set `self.active` false)
  (set `PlayerController.bShowMouseCursor` false (`GameplayStatics.GetPlayerController` 0))
  (`/Engine/EditorBlueprintResources/StandardMacros.IsValid` (stale `InputAction|Interact` _returnvalue)
    (:`Is Valid`
      (`Widget.RemoveFromParent` (stale `InputAction|Interact` _returnvalue))
      (`GameplayStatics.SetGamePaused` false :!pinned true) ; [Gameplay] The title may get paused upon pressing [EXIT] button in Save Station
      (`/Engine/EditorBlueprintResources/StandardMacros.DoOnce` false :!label _label_5
        (:`Completed`
          (`GameplayStatics.PlaySound2D` "/Game/AUDIO/SFX_UI/SW_UI_SaveLoad.SW_UI_SaveLoad" 1.0 0.6 0.065 null null)
          (`|ExecutionSequence`
            (:`then_0`
              (goto _label_4))
            (:`then_1`
              (`KismetSystemLibrary.Delay` 1.0)
              (goto _label_5 :!via `Reset`))))))
    (:`Is Not Valid`
      (goto _label_4))))

(fn `UserConstructionScript`
  (`MeshComponent.SetScalarParameterValueOnMaterials` (`self.SM_terminal`) "Time" 0.0)
  (bind _outactors (`GameplayStatics.GetAllActorsOfClass` "BP_SaveLoad_Station_C"))
  (for (_array_element _array_index) _outactors
    (if (== _array_element self)
      (set `self.station` (+ _array_index 1)))))