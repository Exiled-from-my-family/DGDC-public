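; BP_Dylan_Notes is an interactable trigger that shows notes attributed to the hacker M4NTAL, drawn from the LoadingScreenText array.
; When the player character enters the box, it creates a persistent UI_GenericMessage widget and opens a gate on Interact input.
; Each press cycles to the next note, wrapping around; leaving removes the widget, closes the gate and resets the DoOnce.
; The construction script gives the Radius component a glowing control-point material.
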(event `InputAction|Interact` :consume false
  (params (Key :type "Key Structure"))
  (bind _loading_screen_text (`self.loading screen text`))
  (bind _index (`self.index`))
  (:`Pressed`
    (`/Engine/EditorBlueprintResources/StandardMacros.Gate` true :!label _label
      (:`Exit`
        (`/Engine/EditorBlueprintResources/StandardMacros.IncrementInt` _index
          (:`  `
            (if (>= _index (`KismetArrayLibrary.Array_Length` _loading_screen_text))
              (set `self.index` 0))
            (set `/Game/Blueprints/UI/UI_Pickups/UI_GenericMessage.Message` (`KismetTextLibrary.Conv_StringToText` (`KismetStringLibrary.Concat_StrStr` "Notes written by the hacker known as M4NTAL (interact to cycle). \n \n" (`KismetTextLibrary.Conv_TextToString` (`|GetArrayItem` _loading_screen_text _index)))) (stale `self.Box.OnComponentBeginOverlap` _returnvalue))))))))

(event `self.Box.OnComponentBeginOverlap`
  (params (OverlappedComponent :type "PrimitiveComponent Object Reference") (OtherActor :type "Actor Object Reference") (OtherComp :type "PrimitiveComponent Object Reference") (OtherBodyIndex :type Integer) (bFromSweep :type Boolean) (SweepResult :type "HitResult Structure (by ref)"))
  (cast `/Game/Blueprints/CHARACTERS/fpsMovementCharacter_light_1_vq3` OtherActor)
  (`/Engine/EditorBlueprintResources/StandardMacros.DoOnce` false :!label _label_2
    (:`Completed`
      (bind _returnvalue (`|CreateWidget` "/Game/Blueprints/UI/UI_Pickups/UI_GenericMessage.UI_GenericMessage_C" (`GameplayStatics.GetPlayerController` 0) (`KismetTextLibrary.Conv_StringToText` (`KismetStringLibrary.Concat_StrStr` "Notes written by the hacker known as M4NTAL (interact to cycle). \n \n" (`KismetTextLibrary.Conv_TextToString` (`|GetArrayItem` (`self.loading screen text`) (`self.index`))))) 0.0 false))
      (`UserWidget.AddToViewport` _returnvalue 0)
      (goto _label :!via `Open`))))

(event `self.Box.OnComponentEndOverlap`
  (params (OverlappedComponent :type "PrimitiveComponent Object Reference") (OtherActor :type "Actor Object Reference") (OtherComp :type "PrimitiveComponent Object Reference") (OtherBodyIndex :type Integer))
  (cast `/Game/Blueprints/CHARACTERS/fpsMovementCharacter_light_1_vq3` OtherActor)
  (`Widget.RemoveFromParent` (stale `self.Box.OnComponentBeginOverlap` _returnvalue))
  (`|ExecutionSequence`
    (:`then_0`
      (goto _label_2 :!via `Reset`))
    (:`then_1`
      (goto _label :!via `Close`))))

(fn `UserConstructionScript`
  (bind _radius (`self.Radius`))
  (`PrimitiveComponent.SetMaterial` _radius 0 "/Game/Blueprints/PICKUPS/M_ControlPointRadius_Inst1.M_ControlPointRadius_Inst1")
  (`MeshComponent.SetScalarParameterValueOnMaterials` _radius "Emissive" 6.0))