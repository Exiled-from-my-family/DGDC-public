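; An exploding barrel actor that detonates once when its Destructible component fractures.
; The BOOM event removes the destructible and fires a radial impulse, crater decal, explosion particles, sound, radial damage and world camera shake.
; In parallel, a Shockwave timeline scales up a Plane component, then destroys it when finished.
; The actor destroys itself after a delay.
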(event `self.Destructible.OnComponentFracture`
  (params (HitPoint :type "Vector Structure (by ref)") (HitDirection :type "Vector Structure (by ref)"))
  (`/Engine/EditorBlueprintResources/StandardMacros.DoOnce` false
    (:`Completed`
      (`self.BOOM`))))

(event `BOOM`
  (bind _returnvalue (`self.K2_GetActorLocation`))
  (bind _plane (`self.Plane`))
  (bind _returnvalue_2 (+ _returnvalue (0.0 0.0 135.0)))
  (`|ExecutionSequence`
    (:`then_0`
      (`ActorComponent.K2_DestroyComponent` (`self.Destructible`))
      (`RadialForceComponent.FireImpulse` (`self.RadialForce`))
      (`GameplayStatics.SpawnDecalAtLocation` "/Game/kosm_fps_assets/Misc/Materials/D_Crater.D_Crater" (200.0 200.0 200.0) _returnvalue (struct :`Pitch` -90.0) 30.0)
      (`GameplayStatics.SpawnEmitterAtLocation` "/Game/kosm_fps_assets/Misc/Particles/P_Explode1.P_Explode1" _returnvalue_2 (struct) (6.0 6.0 6.0))
      (`GameplayStatics.SpawnEmitterAtLocation` "/Game/kosm_fps_assets/Misc/Particles/P_Explode4.P_Explode4" _returnvalue_2 (struct) (2.0 2.0 2.0))
      (`GameplayStatics.PlaySoundAtLocation` "/Game/AUDIO/SFX_Weapons/Weap_GrenadeLauncher/SC_Explosion.SC_Explosion" _returnvalue_2 (struct) 1.0 1.0 0.0 null null null)
      (`GameplayStatics.ApplyRadialDamage` :`BaseDamage` 50.0 :`Origin` _returnvalue_2 :`DamageRadius` 1000.0 :`DamageCauser` null :`InstigatedByController` null :`DamagePreventionChannel` "ECC_Camera")
      (`GameplayStatics.PlayWorldCameraShake` "/Game/Blueprints/SHAKES/BP_CameraShake_Explosion.BP_CameraShake_Explosion_C" _returnvalue_2 900.0 4000.0 0.5)
      (`KismetSystemLibrary.Delay` 15.0)
      (`self.K2_DestroyActor`))
    (:`then_1`
      (bind (_direction _expansion) (`Timeline|Shockwave` :!via `PlayFromStart`)
        (:`Update`
          (`SceneComponent.SetWorldScale3D` _plane (`KismetMathLibrary.Conv_DoubleToVector` (`KismetMathLibrary.Lerp` 0.0 20.0 _expansion))))
        (:`Finished`
          (`ActorComponent.K2_DestroyComponent` _plane))))))

(fn `UserConstructionScript`)