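; BP_Gibs_Robot is a short-lived gib effect that scatters robot debris over a crater decal.
; On BeginPlay it takes a random yaw, fires a radial force impulse and sets the crater decal material.
; After five seconds it toggles the visibility of its five gib components, then destroys itself 25 seconds later.
; A random blood-stain decal selection is left unconnected.
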(event `self.ReceiveBeginPlay`
  (`self.K2_SetActorRotation` (`KismetMathLibrary.MakeRotator` 0.0 0.0 (`KismetMathLibrary.RandomFloatInRange` 0.0 180.0)))
  (`RadialForceComponent.FireImpulse` (`self.RadialForce`))
  (`DecalComponent.SetDecalMaterial` (`self.Decal`) "/Game/kosm_fps_assets/Misc/Materials/D_Crater.D_Crater")
  (`KismetSystemLibrary.Delay` 5.0)
  (`SceneComponent.ToggleVisibility` (`self.Gib2`) true)
  (`SceneComponent.ToggleVisibility` (`self.Gib1`) true)
  (`SceneComponent.ToggleVisibility` (`self.Gib4`) true)
  (`SceneComponent.ToggleVisibility` (`self.Gib5`) true)
  (`SceneComponent.ToggleVisibility` (`self.Gib3`) true)
  (`KismetSystemLibrary.Delay` 25.0)
  (`self.K2_DestroyActor`))

(fn `UserConstructionScript`)