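; BP_AutoCheckpoint is a one-shot trigger volume that sets the player's respawn point when fpsMovementCharacter_light_1_vq3 overlaps it.
; On overlap it spawns a Spawnpoint and moves every Spawnpoint in the level to its own transform, then destroys itself.
; It clears message widgets and, if DisplayMessage is set, shows a "checkpoint reached" widget with a sound.
; The construction script sizes the box from TriggerSize and raises it to rest on the actor's origin.
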(event `self.Box.OnComponentBeginOverlap`
  (params (OverlappedComponent :type "PrimitiveComponent Object Reference") (OtherActor :type "Actor Object Reference") (OtherComp :type "PrimitiveComponent Object Reference") (OtherBodyIndex :type Integer) (bFromSweep :type Boolean) (SweepResult :type "HitResult Structure (by ref)"))
  (cast `/Game/Blueprints/CHARACTERS/fpsMovementCharacter_light_1_vq3` OtherActor)
  (`/Engine/EditorBlueprintResources/StandardMacros.DoOnce` false
    (:`Completed`
      (`|SpawnActorFromClass` "/Game/Blueprints/spawnpoint.spawnpoint_C" (`self.GetTransform`) "Undefined" "OverrideRootScale" null null)
      (bind _outactors (`GameplayStatics.GetAllActorsOfClass` "/Game/Blueprints/spawnpoint.spawnpoint_C"))
      (for _array_element _outactors
        (`self.K2_SetActorLocationAndRotation` _array_element (`self.K2_GetActorLocation`) (`self.K2_GetActorRotation`) false false))
      (`/Game/Blueprints/NewFunctionLibrary.clean all message widgets`)
      (bind _returnvalue (`|CreateWidget` "/Game/Blueprints/UI/UI_Pickups/UI_GenericMessage_alt.UI_GenericMessage_alt_C" null "checkpoint reached"))
      (if (`self.display message`)
        (`GameplayStatics.PlaySound2D` "/Game/AUDIO/SFX_UI/Moving_In_Menu/SW_MovingForwardInMenu_05_Variation_01.SW_MovingForwardInMenu_05_Variation_01" 1.0 1.0 0.0 null null)
        (`UserWidget.AddToViewport` _returnvalue 0))
      (`self.K2_DestroyActor`))))

(fn `UserConstructionScript`
  (bind _box (`self.Box`))
  (bind _trigger_size (`self.Trigger size`))
  (`BoxComponent.SetBoxExtent` _box _trigger_size true)
  (`SceneComponent.K2_SetRelativeLocation` _box (`KismetMathLibrary.MakeVector` 0.0 0.0 (.z _trigger_size)) false false))