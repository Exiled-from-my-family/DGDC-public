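; Interactable terminal that fires an interaction event when the player presses Interact nearby, or when force-activated.
; Tick polls the box overlap to show a key-binding prompt and open a gate that lets the input through.
; Activation runs once, swapping material, playing a sound, removing the prompt and disabling player controller input; Repeat re-arms it after a delay.
; The construction script creates dynamic materials for the mesh.
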(event `self.ReceiveBeginPlay`)

(event `force activate`
  (bind _returnvalue (`GameplayStatics.GetPlayerController` 0))
  (`/Engine/EditorBlueprintResources/StandardMacros.DoOnce` false :!label _label
    (:`Completed`
      (set `self.active` true)
      (`GameplayStatics.PlaySound2D` (`self.SFX`) 1.0 1.0 0.0 null null)
      (`PrimitiveComponent.SetMaterial` (`self.SM_Interactable`) (`self.Material slot`) (`self.Material_Interacted_Post`))
      (`self.InteractionEvent`)
      (`/Engine/EditorBlueprintResources/StandardMacros.IsValid` (stale `self.ReceiveTick` _returnvalue)
        (:`Is Valid`
          (`Widget.RemoveFromParent` (stale `self.ReceiveTick` _returnvalue)))
        (:`Is Not Valid`
          _))
      (`self.DisableInput` _returnvalue _returnvalue)
      (if (`self.Repeat?`)
        (`KismetSystemLibrary.Delay` (`self.Delay for repeat`))
        (set `self.active` false)
        (`PrimitiveComponent.SetMaterial` (`self.SM_Interactable`) (`self.Material slot`) (`self.Material_Interacted_Pre`))
        (goto _label :!via `Reset`)))))

(event `self.ReceiveTick`
  (params (DeltaSeconds :type "Float (single-precision)"))
  (`/Engine/EditorBlueprintResources/StandardMacros.IsValid` (`|GetArrayItem` (`PrimitiveComponent.GetOverlappingActors` (`self.Box`) "/Game/Blueprints/CHARACTERS/fpsMovementCharacter_light_1_vq3.fpsMovementCharacter_light_1_vq3_C"))
    (:`Is Valid`
      (`/Engine/EditorBlueprintResources/StandardMacros.DoOnce` false :!label _label_2
        (:`Completed`
          (set `self.IsNear?` true)
          (if (not (`self.active`))
            (bind _returnvalue (`|CreateWidget` "/Game/Blueprints/UI/UI_Pickups/UI_GenericMessage_alt.UI_GenericMessage_alt_C" (`GameplayStatics.GetPlayerController` 0) (`KismetTextLibrary.Conv_StringToText` (`KismetStringLibrary.Concat_StrStr` "press [" (`KismetTextLibrary.Conv_TextToString` (`/Game/Blueprints/NewFunctionLibrary.gamepad or keyboard func` (`InputSettings.GetActionMappingByName` (`InputSettings.GetInputSettings`) "Interact"))) "] to " (`self.action`))) 1.5 false))
            (`MeshComponent.SetScalarParameterValueOnMaterials` (`self.SM_Interactable`) "Time" 1.0)
            (`UserWidget.AddToViewport` _returnvalue 0)
            (goto _label_3 :!via `Open`)))))
    (:`Is Not Valid`
      (`|ExecutionSequence`
        (:`then_0`
          (`/Engine/EditorBlueprintResources/StandardMacros.IsValid` _returnvalue
            (:`Is Valid`
              (`Widget.RemoveFromParent` _returnvalue)
              (goto _label_3 :!via `Close`))
            (:`Is Not Valid`
              (goto _label_3 :!via `Close`))))
        (:`then_1`
          (goto _label_2 :!via `Reset`))))))

(event `InputAction|Interact` :consume false
  (params (Key :type "Key Structure"))
  (:`Pressed`
    (`/Engine/EditorBlueprintResources/StandardMacros.Gate` true :!label _label_3
      (:`Exit`
        (if (and (`self.IsNear?`) (not (`self.active`)))
          (goto _label))))))

(fn `UserConstructionScript`
  (`PrimitiveComponent.CreateDynamicMaterialInstance` (`self.SM_Interactable`) 0 (`self.Material0`) "None")
  (`PrimitiveComponent.CreateDynamicMaterialInstance` (`self.SM_Interactable`) 1 (`self.Material1`) "None")
  (if (`self.more materials?`)
    (`PrimitiveComponent.CreateDynamicMaterialInstance` (`self.SM_Interactable`) 2 (`self.Material2`) "None")))