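; BP_WaterBody is a water volume that reacts to characters entering and leaving its Box trigger.
; On entry it spawns a splash emitter below any Character and plays a dive sound if that character is falling fast enough.
; It also switches FootstepsType on fpsMovementCharacter_light_1_vq3 while inside, resetting it when the overlap ends.
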(event `self.Box.OnComponentBeginOverlap`
  (params (OverlappedComponent :type "PrimitiveComponent Object Reference") (OtherActor :type "Actor Object Reference") (OtherComp :type "PrimitiveComponent Object Reference") (OtherBodyIndex :type Integer) (bFromSweep :type Boolean) (SweepResult :type "HitResult Structure (by ref)"))
  (`|ExecutionSequence`
    (:`then_0`
      (bind _ascharacter (cast `Character` OtherActor))
      (if (< (.z (`self.GetVelocity` _ascharacter)) -1500.0)
        (bind _returnvalue (`self.K2_GetActorLocation` _ascharacter))
        (`GameplayStatics.PlaySoundAtLocation` "/Game/AUDIO/SFX_Ambient/SC_WaterDive.SC_WaterDive" _returnvalue (struct) 1.0 1.0 0.0 "/Game/kosm_fps_assets/Misc/SoundFX/SoundAttenuationNormal.SoundAttenuationNormal" null null))
      (`GameplayStatics.SpawnEmitterAtLocation` "/Game/kosm_fps_assets/Misc/Particles/P_Splash.P_Splash" (- _returnvalue (0.0 0.0 150.0)) (struct) (2.0 2.0 2.0)))
    (:`then_1`
      (bind _asfps_movement_character_light_1_vq_3 (cast `/Game/Blueprints/CHARACTERS/fpsMovementCharacter_light_1_vq3` OtherActor))
      (set `/Game/Blueprints/CHARACTERS/fpsMovementCharacter_light_1_vq3.Footsteps_Type` 1 _asfps_movement_character_light_1_vq_3))))

(event `self.Box.OnComponentEndOverlap`
  (params (OverlappedComponent :type "PrimitiveComponent Object Reference") (OtherActor :type "Actor Object Reference") (OtherComp :type "PrimitiveComponent Object Reference") (OtherBodyIndex :type Integer))
  (`|ExecutionSequence`
    (:`then_0`
      (cast `Character` OtherActor))
    (:`then_1`
      (bind _asfps_movement_character_light_1_vq_3 (cast `/Game/Blueprints/CHARACTERS/fpsMovementCharacter_light_1_vq3` OtherActor))
      (set `/Game/Blueprints/CHARACTERS/fpsMovementCharacter_light_1_vq3.Footsteps_Type` 0 _asfps_movement_character_light_1_vq_3))))

(fn `UserConstructionScript`)