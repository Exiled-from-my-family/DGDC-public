(event `self.ReceiveBeginPlay`
  (bind _unlocked_ (`/Game/Blueprints/NewFunctionLibrary.has unlockable` (`self.Secret unlockable`)))
  (if _unlocked_
    (`self.K2_DestroyActor`)))

(event `self.Box.OnComponentBeginOverlap`
  (params (OverlappedComponent :type "PrimitiveComponent Object Reference") (OtherActor :type "Actor Object Reference") (OtherComp :type "PrimitiveComponent Object Reference") (OtherBodyIndex :type Integer) (bFromSweep :type Boolean) (SweepResult :type "HitResult Structure (by ref)"))
  (cast `/Game/Blueprints/CHARACTERS/fpsMovementCharacter_light_1_vq3` OtherActor)
  (`/Engine/EditorBlueprintResources/StandardMacros.DoOnce` false
    (:`Completed`
      (bind _returnvalue (`|CreateWidget` "/Game/Blueprints/UI/UI_Pickups/UI_GenericMessage_alt.UI_GenericMessage_alt_C" null "you found a secret!"))
      (`UserWidget.AddToViewport` _returnvalue 0)
      (`GameplayStatics.PlaySound2D` "/Game/MISSIONS/EP1/Audio/SC_Secret.SC_Secret" 0.4 1.0 0.0 null null)
      (`/Game/Blueprints/NewFunctionLibrary.add unlockable` (`self.Secret unlockable`))
      (bind _outactors (`GameplayStatics.GetAllActorsOfClass` "BP_SecretMessage_C"))
      (for _array_element _outactors
        (if (`KismetStringLibrary.EqualEqual_StrStr` (`/Game/Blueprints/MISC/BP_SecretMessage.Secret unlockable` _array_element) (`self.Secret unlockable`))
          (`self.K2_DestroyActor` _array_element)))
      (`KismetSystemLibrary.Delay` 1.0)
      (`self.K2_DestroyActor`))))

(fn `UserConstructionScript`)