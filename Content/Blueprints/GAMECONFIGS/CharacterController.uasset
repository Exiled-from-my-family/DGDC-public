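; Player controller that lets the player pick a VQ3 or CPMA movement character from a selection widget.
; Tick binds both buttons every frame while the widget is valid; clicks run paired Server/Client events and add the matching HUD on authority.
; Server events spawn the character with GameMode team data, replace CharacterSelected and possess it via player index 0.
; Client events restore game-only input; the menu-toggle logic is unconnected.
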(event `self.ReceiveTick`
  (params (DeltaSeconds :type "Float (single-precision)"))
  (bind _characterselectionwidget (`self.CharacterSelectionWidget`))
  ;[1 1 1] Character Selection
  (`/Engine/EditorBlueprintResources/StandardMacros.IsValid` _characterselectionwidget
    (:`Is Valid`
      (add `Button.OnClicked` (`/Game/Blueprints/UI/CharacterSelection.Button_203` _characterselectionwidget) (delegate `OnClicked_Event_VQ3`))
      (add `Button.OnClicked` (`/Game/Blueprints/UI/CharacterSelection.Button` _characterselectionwidget) (delegate `OnClicked_Event_CPMA`)))))

(event `OnClicked_Event_VQ3`
  ;[1 1 1] Character Selection
  (`WidgetLayoutLibrary.RemoveAllWidgets`)
  (`self.VQ3SelectionServer`)
  (`self.VQ3SelectionClient`)
  (`/Engine/EditorBlueprintResources/ActorMacros.Switch Has Authority`
    (:`Authority`
      (bind _returnvalue (`|CreateWidget` "/Game/Blueprints/UI/HUD_vq3.HUD_vq3_C" (`Widget.GetOwningPlayer` (`self.CharacterSelectionWidget`))))
      (`UserWidget.AddToViewport` _returnvalue 0))))

(event `OnClicked_Event_CPMA`
  ;[1 1 1] Character Selection
  (`WidgetLayoutLibrary.RemoveAllWidgets`)
  (`self.CPMASelectionServer`)
  (`self.CPMASelectionClient`)
  (`/Engine/EditorBlueprintResources/ActorMacros.Switch Has Authority`
    (:`Authority`
      (bind _returnvalue (`|CreateWidget` "/Game/Blueprints/UI/HUD_cpma.HUD_cpma_C" (`Widget.GetOwningPlayer` (`self.CharacterSelectionWidget`))))
      (`UserWidget.AddToViewport` _returnvalue 0))))

(event `VQ3SelectionServer`
  (bind _returnvalue (`GameplayStatics.GetPlayerCharacter` 0))
  (bind _returnvalue_2 (`GameplayStatics.GetPlayerController` 0))
  (bind _askosm_game_mode (cast `/Game/Blueprints/GAMECONFIGS/Kosm_GameMode` (`GameplayStatics.GetGameMode`) :!pure true))
  ;[1 1 1] Character Selection
  ;;[0.007223 1 0] VQ3
  (bind _returnvalue_3 (`|SpawnActorFromClass` "/Game/Blueprints/CHARACTERS/fpsMovementCharacter_light_1_vq3.fpsMovementCharacter_light_1_vq3_C" (`self.GetTransform` _returnvalue) "AlwaysSpawn" "OverrideRootScale" _returnvalue (`/Game/Blueprints/GAMECONFIGS/Kosm_GameMode.TeamPC` _askosm_game_mode) (`KismetMathLibrary.Conv_VectorToLinearColor` (`/Game/Blueprints/GAMECONFIGS/Kosm_GameMode.TeamVar` _askosm_game_mode)) _returnvalue))
  (`self.K2_DestroyActor` (`/Game/Blueprints/GAMECONFIGS/Kosm_GameMode.CharacterSelected` _askosm_game_mode))
  (set `/Game/Blueprints/GAMECONFIGS/Kosm_GameMode.CharacterSelected` _returnvalue_3 _askosm_game_mode)
  (`self.UnPossess` _returnvalue_2)
  (`self.Possess` _returnvalue_2 _returnvalue_3)
  (`self.SetOwner` _returnvalue_3 _returnvalue_2))

(event `VQ3SelectionClient`
  (bind _returnvalue (`GameplayStatics.GetPlayerController` 0))
  ;[1 1 1] Character Selection
  ;;[0.007223 1 0] VQ3
  (`WidgetBlueprintLibrary.SetInputMode_GameOnly` _returnvalue)
  (set `PlayerController.bShowMouseCursor` false _returnvalue)
  (set `/Game/Blueprints/UI/CharacterSelection.WidgetOpen` true (`self.CharacterSelectionWidget`))
  (`Widget.RemoveFromParent` (`self.CharacterSelectionWidget`))
  (`KismetSystemLibrary.PrintString` "VQ3 spawned"))

(event `CPMASelectionServer`
  (bind _returnvalue (`GameplayStatics.GetPlayerController` 0))
  (bind _returnvalue_2 (`GameplayStatics.GetPlayerPawn` 0))
  (bind _askosm_game_mode (cast `/Game/Blueprints/GAMECONFIGS/Kosm_GameMode` (`GameplayStatics.GetGameMode`) :!pure true))
  ;[1 1 1] Character Selection
  ;;[1 0 0] CPMA
  (bind _returnvalue_3 (`|SpawnActorFromClass` "/Game/Blueprints/CHARACTERS/fpsMovementCharacter_light_2_cpma.fpsMovementCharacter_light_2_cpma_C" (`self.GetTransform` _returnvalue_2) "AlwaysSpawn" "OverrideRootScale" _returnvalue_2 (`/Game/Blueprints/GAMECONFIGS/Kosm_GameMode.TeamPC` _askosm_game_mode) (`KismetMathLibrary.Conv_VectorToLinearColor` (`/Game/Blueprints/GAMECONFIGS/Kosm_GameMode.TeamVar` _askosm_game_mode)) _returnvalue_2))
  (`self.K2_DestroyActor` (`/Game/Blueprints/GAMECONFIGS/Kosm_GameMode.CharacterSelected` _askosm_game_mode))
  (set `/Game/Blueprints/GAMECONFIGS/Kosm_GameMode.CharacterSelected` _returnvalue_3 _askosm_game_mode)
  (`self.UnPossess` _returnvalue)
  (`self.Possess` _returnvalue _returnvalue_3)
  (`self.SetOwner` _returnvalue_3 _returnvalue))

(event `CPMASelectionClient`
  (bind _returnvalue (`GameplayStatics.GetPlayerController` 0))
  ;[1 1 1] Character Selection
  ;;[1 0 0] CPMA
  (`WidgetBlueprintLibrary.SetInputMode_GameOnly` _returnvalue)
  (set `PlayerController.bShowMouseCursor` false _returnvalue)
  (set `/Game/Blueprints/UI/CharacterSelection.WidgetOpen` true (`self.CharacterSelectionWidget`))
  (`Widget.RemoveFromParent` (`self.CharacterSelectionWidget`))
  (`KismetSystemLibrary.PrintString` "CPMA spawned"))

(fn `UserConstructionScript`)