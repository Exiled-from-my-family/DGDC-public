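; Game mode for Kosm that spawns and possesses the FPS character with a random team color and handles map arrival.
; Player start selection prefers a PIE start, then an unused portal matching the last visited map, then any unused PlayerStart.
; BeginPlay updates map history, force-unlocks a hardcoded level list, and after a load preserves weapon/ammo and teleports to the saved station.
; In non-packaged builds, Interact skips movie dialogue.
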(event `InputAction|Interact` :consume false
  (params (Key :type "Key Structure"))
  (:`Pressed`
    (if (not (`KismetSystemLibrary.IsPackagedForDistribution`))
      (`/Game/Blueprints/NewFunctionLibrary.SKIP MOVIE DIALOGUE`))))

(event `self.ReceiveBeginPlay`
  (`|ExecutionSequence`
    (:`then_0`
      (bind _game_instance (`/Game/Blueprints/NewFunctionLibrary.dead game instance`))
      (if (`/Game/Blueprints/DeadGaemInstance.loaded?` _game_instance)
        (set `/Game/Blueprints/DeadGaemInstance.weapon slot instance, for reals only temp` (`/Game/Blueprints/DeadGaemInstance.weapon slot instance, for reals only` _game_instance) _game_instance)
        (set `/Game/Blueprints/DeadGaemInstance.ammo value temp` (`/Game/Blueprints/DeadGaemInstance.ammo values` _game_instance) _game_instance))
      (`KismetSystemLibrary.Delay` 0.2)
      (bind _returnvalue (`GameplayStatics.GetCurrentLevelName` true))
      (set `/Game/Blueprints/DeadGaemInstance.last map visited persistant` (stale _output_get) _game_instance)
      (bind _output_get (set `/Game/Blueprints/DeadGaemInstance.last map visited` (`KismetStringLibrary.Conv_StringToName` _returnvalue) _game_instance))
      (`KismetSystemLibrary.PrintString` _returnvalue true true (struct :`R` 1.0 :`G` 0.038692 :`A` 1.0))
      (if (`/Game/Blueprints/DeadGaemInstance.loaded?` _game_instance)
        (bind _outactors (`GameplayStatics.GetAllActorsOfClass` "/Game/Blueprints/MISC/BP_SaveLoad_Station.BP_SaveLoad_Station_C"))
        (for _array_element _outactors
          (if (== (`/Game/Blueprints/MISC/BP_SaveLoad_Station.station` _array_element) (`/Game/Blueprints/DeadGaemInstance.station` _game_instance))
            (`self.K2_SetActorTransform` (`/Game/Blueprints/NewFunctionLibrary.get player PURE`) (`SceneComponent.K2_GetComponentToWorld` (`/Game/Blueprints/MISC/BP_SaveLoad_Station.Billboard` _array_element)) false true)))
        (set `/Game/Blueprints/DeadGaemInstance.loaded?` false _game_instance)))
    (:`then_1`
      (for _array_element_2 (`|MakeArray` "DOM_1" "DOM_2" "DOM_3" "EP3_CTF1" "EP3_CTF2" "EP3_CTF3" "EP3_HUB" "EP4_Abandoned" "EP2_HUBend" "EP3_HubEndingDialogue" "CTF_HUB_dialogue" "" "" "" "" :!type "Text") :!pinned true
        (`/Game/Blueprints/NewFunctionLibrary.add unlockable` (`KismetTextLibrary.Conv_TextToString` _array_element_2))))))

(event `self.K2_PostLogin`
  (params (NewPlayer :type "PlayerController Object Reference"))
  (bind _output_get (set `self.TeamVar` (`KismetMathLibrary.Vector_GetAbs` (`KismetMathLibrary.RandomUnitVector`))))
  (bind _returnvalue (`|SpawnActorFromClass` "/Game/Blueprints/CHARACTERS/fpsMovementCharacter_light_1_vq3.fpsMovementCharacter_light_1_vq3_C" (`self.GetTransform` (`self.K2_FindPlayerStart` NewPlayer)) "AdjustIfPossibleButAlwaysSpawn" "OverrideRootScale" NewPlayer NewPlayer (`KismetMathLibrary.Conv_VectorToLinearColor` _output_get) null))
  (set `self.CharacterSelected` _returnvalue)
  (`Controller.Possess` NewPlayer _returnvalue))

(fn `ChoosePlayerStart`
  (params (Player :type "Controller Object Reference"))
  (returns (ReturnValue :type "Actor Object Reference"))
  (bind _outactors (`GameplayStatics.GetAllActorsOfClass` "/Script/Engine.PlayerStartPIE"))
  (if (`KismetMathLibrary.Conv_IntToBool` (`KismetArrayLibrary.Array_Length` _outactors))
    (return (`|GetArrayItem` _outactors))
    (else
      (bind _game_instance (`/Game/Blueprints/NewFunctionLibrary.dead game instance`))
      (bind _outactors_2 (`GameplayStatics.GetAllActorsOfClass` "/Game/MISSIONS/EP0/Blueprints/player_start_portal.player_start_portal_C"))
      (for _array_element _outactors_2
        (bind _last_map_visited (`/Game/Blueprints/DeadGaemInstance.last map visited` _game_instance))
        (if (and (!= (`PlayerStart.PlayerStartTag` _array_element) "Spawned") (or (== (`/Game/MISSIONS/EP0/Blueprints/player_start_portal.revisit` _array_element) _last_map_visited) (== (`/Game/MISSIONS/EP0/Blueprints/player_start_portal.map name` _array_element) _last_map_visited)))
          (`|ExecutionSequence`
            (:`then_0`
              (set `PlayerStart.PlayerStartTag` "Spawned" _array_element))
            (:`then_1`
              (return _array_element)))))
      (bind _outactors_3 (`GameplayStatics.GetAllActorsOfClass` "/Script/Engine.PlayerStart"))
      (for _array_element_2 _outactors_3
        (if (!= (`PlayerStart.PlayerStartTag` _array_element_2) "Spawned")
          (`|ExecutionSequence`
            (:`then_0`
              (break))
            (:`then_1`
              (set `PlayerStart.PlayerStartTag` "Spawned" _array_element_2))
            (:`then_2`
              (return _array_element_2))))))))

(fn `UserConstructionScript`)