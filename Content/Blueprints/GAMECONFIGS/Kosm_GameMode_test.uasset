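; Test game mode that spawns and possesses an FpsMovementCharacter_light_2_cpma pawn for each player who logs in.
; PostLogin places the pawn at the found player start, passing the controller and a random team color built from an absolute unit vector.
; The ChoosePlayerStart override hands out the first PlayerStart not tagged "Spawned" and tags it, so each start is used once.
; A second, offset spawn is left unconnected.
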(event `self.ReceiveBeginPlay`)

(event `self.K2_PostLogin`
  (params (NewPlayer :type "PlayerController Object Reference"))
  (bind _output_get (set `self.TeamVar` (`KismetMathLibrary.Vector_GetAbs` (`KismetMathLibrary.RandomUnitVector`))))
  (bind _returnvalue (`|SpawnActorFromClass` "/Game/Blueprints/CHARACTERS/fpsMovementCharacter_light_2_cpma.fpsMovementCharacter_light_2_cpma_C" (`self.GetTransform` (`self.K2_FindPlayerStart` NewPlayer)) "AdjustIfPossibleButAlwaysSpawn" "OverrideRootScale" NewPlayer NewPlayer (`KismetMathLibrary.Conv_VectorToLinearColor` _output_get) null))
  (set `self.CharacterSelected` _returnvalue)
  (`Controller.Possess` NewPlayer _returnvalue))

(fn `ChoosePlayerStart`
  (params (Player :type "Controller Object Reference"))
  (returns (ReturnValue :type "Actor Object Reference"))
  (bind _outactors (`GameplayStatics.GetAllActorsOfClass` "/Script/Engine.PlayerStart"))
  (for _array_element _outactors
    (if (!= (`PlayerStart.PlayerStartTag` _array_element) "Spawned")
      (`|ExecutionSequence`
        (:`then_0`
          (break))
        (:`then_1`
          (set `PlayerStart.PlayerStartTag` "Spawned" _array_element))
        (:`then_2`
          (return _array_element))))))

(fn `UserConstructionScript`)