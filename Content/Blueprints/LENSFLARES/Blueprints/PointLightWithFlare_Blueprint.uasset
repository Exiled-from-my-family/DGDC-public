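; Point light actor Blueprint that renders a lens flare through a particle system matched to the light's color and intensity.
; The construction script applies color and intensity to the PointLight, then calls InitFlares, which BeginPlay also runs.
; InitFlares puts a dynamic instance of FlaresMaterial on the particle system, setting corrected intensity, depth offset, camera distance and emitter size.
; Flare color, size and rotation pass through particle instance parameters.
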(event `self.ReceiveBeginPlay`
  ;[1 1 1] Init Flares
  (`self.InitFlares`))

(fn `InitFlares`
  ;[1 1 1] Creates new Dynamic material instance, that will be assigned to particle
  (bind _returnvalue (`KismetMaterialLibrary.CreateDynamicMaterialInstance` (`self.ParticleSystem`) (`self.FlaresMaterial`)))
  ;[1 1 1] This variable is made for comfort
  (set `self.MaterialInstance` _returnvalue)
  ;[1 1 1] Assigns material to first slot of particle system. If particle doesn't exist, this node won't be completed and further execution will be interrupted, accordingly to blueprint execution process rules.
  (`PrimitiveComponent.SetMaterial` (`self.ParticleSystem`) 0 (`self.MaterialInstance`))
  ;[1 1 1] This nodes set all parameters for effect
  (`|ExecutionSequence`
    (:`then_0`
      ;;[1 1 1] Setup light intensity correction for PointLight
      (`MaterialInstanceDynamic.SetScalarParameterValue` (`self.MaterialInstance`) "FlareIntensity" (* (`LightComponentBase.Intensity` (`self.PointLight`)) (`self.FlareIntensityCorrection`))))
    (:`then_1`
      ;;[1 1 1] Sets the Depth Offset parameter to correct effect position in depth buffer
      (`MaterialInstanceDynamic.SetScalarParameterValue` (`self.MaterialInstance`) "DepthOffset" (`self.DepthOffset`)))
    (:`then_2`
      ;;[1 1 1] Sets DistanceToCamera, the distance to camera on which particle will always be, if material with KeepConstantScale parameter is used
      (`MaterialInstanceDynamic.SetScalarParameterValue` (`self.MaterialInstance`) "DistanceToCamera" (`self.DistanceToCamera`)))
    (:`then_3`
      ;;[1 1 1] Setup EmitterSize paramter of material
      (`MaterialInstanceDynamic.SetScalarParameterValue` (`self.MaterialInstance`) "EmitterSize" (`self.EmitterSize`)))
    (:`then_4`
      ;;[1 1 1] Setup Flare Color. It is the same color as one, that is used for the PointLight color
      (`ParticleSystemComponent.SetColorParameter` (`self.ParticleSystem`) "FlareColor" (`LightComponentBase.GetLightColor` (`self.PointLight`))))
    (:`then_5`
      ;;[1 1 1] Setup size of a flare
      (`ParticleSystemComponent.SetVectorParameter` (`self.ParticleSystem`) "FlareSize" (`self.FlareSize`)))
    (:`then_6`
      ;;[1 1 1] Setup rotation for a particle that is spawned by the ParticleSystem component. In other words, this set rotation for a lens flare effect
      (`ParticleSystemComponent.SetFloatParameter` (`self.ParticleSystem`) "Rotation" (/ (`self.Rotation`) 360.0)))
    (:`then_7`
      ;;[1 1 1] Exit from function
      (return))))

(fn `UserConstructionScript`
  ;[1 1 1] Control Light Source
  (`LightComponent.SetLightColor` (`self.PointLight`) (`self.Color`) true) ; Setup Light Color
  (`LightComponent.SetIntensity` (`self.PointLight`) (`self.LightIntensity`)) ; Set up Ligth Intensity
  (`self.InitFlares`) ; Initialize LensFlare Effect
)