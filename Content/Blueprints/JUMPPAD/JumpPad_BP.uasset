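; Jump pad actor that flings characters, physics props and grenade launcher projectiles along a shared JumpStrength vector.
; On overlap, characters are launched with XY and Z velocity override, while barrel and ball physics actors receive a velocity-change impulse on their meshes.
; Grenade launcher projectiles get the same impulse through the Hit event instead.
; Each successful launch plays the jump pad sound at the pad's mesh location.
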(event `self.ReceiveActorBeginOverlap`
  (params (OtherActor :type "Actor Object Reference"))
  (bind (_asphysics_actor_ball_bp _bsuccess) (cast `/Game/Blueprints/PHYSICSOBJECTS/PhysicsActor_BallBP` OtherActor :!pure true))
  (bind (_asphysics_actor_barrel_bp _bsuccess_2) (cast `/Game/Blueprints/PHYSICSOBJECTS/PhysicsActor_BarrelBP` OtherActor :!pure true))
  (bind (_ascharacter _bsuccess_3) (cast `Character` OtherActor :!pure true))
  (if _bsuccess_3
    (`Character.LaunchCharacter` _ascharacter (`self.Jump strength`) true true)
    (`GameplayStatics.PlaySoundAtLocation` "/Game/AUDIO/jumpPad_Cue.jumpPad_Cue" (`SceneComponent.K2_GetComponentLocation` (`self.StaticMeshComponent`)) (struct) 1.0 1.0 0.0 null null null :!label _label)
    (elif _bsuccess_2
      (`PrimitiveComponent.AddImpulse` (`StaticMeshActor.StaticMeshComponent` _asphysics_actor_barrel_bp) (`self.Jump strength`) "None" true)
      (goto _label)
      (elif _bsuccess
        (`PrimitiveComponent.AddImpulse` (`StaticMeshActor.StaticMeshComponent` _asphysics_actor_ball_bp) (`self.Jump strength`) "None" true)
        (goto _label)))))

(event `self.ReceiveHit`
  (params (MyComp :type "PrimitiveComponent Object Reference") (Other :type "Actor Object Reference") (OtherComp :type "PrimitiveComponent Object Reference") (bSelfMoved :type Boolean) (HitLocation :type "Vector Structure") (HitNormal :type "Vector Structure") (NormalImpulse :type "Vector Structure") (Hit :type "HitResult Structure (by ref)"))
  (bind (_asfps_movement_projectile_grenade_launcher _bsuccess) (cast `/Game/Blueprints/PROJECTILES/fpsMovementProjectile_GrenadeLauncher` Other :!pure true))
  (if _bsuccess
    (`PrimitiveComponent.AddImpulse` (`/Game/Blueprints/PROJECTILES/fpsMovementProjectile_GrenadeLauncher.StaticMesh` _asfps_movement_projectile_grenade_launcher) (`self.Jump strength`) "None" true)
    (goto _label)))

(fn `UserConstructionScript`)