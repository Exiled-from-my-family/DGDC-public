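; Small health vial pickup that adds Amount to an overlapping character's health, then hides and optionally respawns after a delay with sound and particles.
; Overlap routes through authority-switched server and multicast events.
; Three character classes get separate checks, caps and health bar updates; only vq3 can overheal to 200, with a do-once guard and pickup message.
; Successful pickups also play a sound and report noise to AI.
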(event `self.ReceiveActorBeginOverlap`
  (params (OtherActor :type "Actor Object Reference"))
  ;[0.3687 0.5739 1] Pickup Overlap
  (`/Engine/EditorBlueprintResources/ActorMacros.Switch Has Authority`
    (:`Authority`
      (`self.HealthPickupMulticast` OtherActor))
    (:`Remote`
      (`self.HealthPickupServer` OtherActor))))

(event `HealthPickupMulticast`
  (params (Actor :type "Actor Object Reference"))
  (bind _returnvalue (`self.K2_GetActorLocation`))
  (bind _returnvalue_2 (`self.K2_GetActorLocation`))
  ;[0.3687 0.5739 1] Pickup Overlap
  (bind _asfps_movement_character_light_1_vq_3 (cast `/Game/Blueprints/CHARACTERS/fpsMovementCharacter_light_1_vq3` Actor)
    (:`then`
      (if (not (`/Game/Blueprints/CHARACTERS/fpsMovementCharacter_light_1_vq3.IsDead?` _asfps_movement_character_light_1_vq_3))
        (bind _health (`/Game/Blueprints/CHARACTERS/fpsMovementCharacter_light_1_vq3.Health` _asfps_movement_character_light_1_vq_3))
        (if (not (>= _health 200.0))
          (`/Engine/EditorBlueprintResources/StandardMacros.DoOnce` false :!label _label
            (:`Completed`
              (bind _output_get (set `/Game/Blueprints/CHARACTERS/fpsMovementCharacter_light_1_vq3.Health` (`KismetMathLibrary.FClamp` (+ _health (`self.amount`)) 0.0 200.0) _asfps_movement_character_light_1_vq_3))
              (message `/Game/Blueprints/UI/UI_Interface.SetHealthBarPercent` (`WidgetComponent.GetUserWidgetObject` (`/Game/Blueprints/CHARACTERS/fpsMovementCharacter_light_1_vq3.HealthBar_3D_WG` _asfps_movement_character_light_1_vq_3)) (/ _output_get 100.0))
              (`GameplayStatics.PlaySoundAtLocation` "/Game/AUDIO/SFX_Pickups/SC_HealthPickup.SC_HealthPickup" _returnvalue (struct) 1.0 1.0 0.0 null null null)
              ;;[1 1 1] Health Widget
              (`/Game/Blueprints/NewFunctionLibrary.clean all message widgets`)
              (`KismetSystemLibrary.Delay` 0.01)
              (bind _returnvalue_3 (`|CreateWidget` "/Game/Blueprints/UI/UI_Pickups/UI_Pickup_Health.UI_Pickup_Health_C"))
              (set `/Game/Blueprints/UI/UI_Pickups/UI_Pickup_Health.Message` "picked up Health Vial (+5)" _returnvalue_3)
              (`UserWidget.AddToViewport` _returnvalue_3 0)
              (`AISense_Hearing.ReportNoiseEvent` (`self.K2_GetActorLocation`) 1.0 _asfps_movement_character_light_1_vq_3)
              (`self.SetActorHiddenInGame` true :!label _label_2)
              (`self.SetActorEnableCollision` false)
              (`KismetSystemLibrary.Delay` (`self.respawn time`))
              (if (`self.respawn?`)
                (`self.SetActorHiddenInGame` false)
                (`self.SetActorEnableCollision` true)
                (`GameplayStatics.PlaySoundAtLocation` "/Game/AUDIO/SFX_Pickups/SC_PickupRespawn.SC_PickupRespawn" _returnvalue_2 (struct) 0.7 1.0 0.0 null null null)
                (`GameplayStatics.SpawnEmitterAtLocation` "/Game/kosm_fps_assets/Misc/Particles/P_LightEmitter1.P_LightEmitter1" (+ _returnvalue_2 (0.0 0.0 65.0)) (struct) (2.5 2.5 2.5))
                (goto _label :!via `Reset`)))))))
    (:`CastFailed`
      (bind _asfps_movement_character_light_2_cpma (cast `/Game/Blueprints/CHARACTERS/fpsMovementCharacter_light_2_cpma` Actor)
        (:`then`
          (bind _health_2 (`/Game/Blueprints/CHARACTERS/fpsMovementCharacter_light_2_cpma.Health` _asfps_movement_character_light_2_cpma))
          (if (not (>= _health_2 100.0))
            (bind _output_get_2 (set `/Game/Blueprints/CHARACTERS/fpsMovementCharacter_light_2_cpma.Health` (`KismetMathLibrary.FClamp` (+ _health_2 (`self.amount`)) 0.0 100.0) _asfps_movement_character_light_2_cpma))
            (message `/Game/Blueprints/UI/UI_Interface.SetHealthBarPercent` (`WidgetComponent.GetUserWidgetObject` (`/Game/Blueprints/CHARACTERS/fpsMovementCharacter_light_2_cpma.HealthBar_3D_WG` _asfps_movement_character_light_2_cpma)) (/ _output_get_2 100.0))
            (`GameplayStatics.PlaySoundAtLocation` "/Game/AUDIO/SFX_Pickups/SC_HealthPickup.SC_HealthPickup" _returnvalue (struct) 1.0 1.0 0.0 null null null :!label _label_3)
            (`AISense_Hearing.ReportNoiseEvent` (`self.K2_GetActorLocation`) 1.0 _asfps_movement_character_light_2_cpma)
            (goto _label_2)))
        (:`CastFailed`
          (bind _asep_1_character (cast `/Game/MISSIONS/EP1/Characters/ep1_character` Actor))
          (if (`/Game/MISSIONS/EP1/Characters/ep1_character.can pick up healthpacks` _asep_1_character)
            (if (not (`/Game/Blueprints/CHARACTERS/NoobotAI/Blueprints/AI_NoobotChar.IsDead?` _asep_1_character))
              (bind _health_3 (`/Game/Blueprints/CHARACTERS/NoobotAI/Blueprints/AI_NoobotChar.Health` _asep_1_character))
              (if (not (or (`self.ActorHasTag` _asep_1_character "Robot") (>= _health_3 100.0)))
                (set `/Game/Blueprints/CHARACTERS/NoobotAI/Blueprints/AI_NoobotChar.Health` (`KismetMathLibrary.FClamp` (+ _health_3 (`self.amount`)) 0.0 100.0) _asep_1_character)
                (`/Game/Blueprints/HEALTHBARS/Blueprints/Widgets/Widget_FloatingHealthbar.AddValue` (`/Game/MISSIONS/EP1/Characters/ep1_character.Get Healthbar` _asep_1_character) "NewEnumerator0" (`self.amount`))
                (goto _label_3)))))))))

(event `HealthPickupServer`
  (params (Actor :type "Actor Object Reference"))
  ;[0.3687 0.5739 1] Pickup Overlap
  (`self.HealthPickupMulticast` Actor))

(fn `UserConstructionScript`)