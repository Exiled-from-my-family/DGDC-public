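; BP_Website_Pickup is a collectible weblink that unlocks a website URL for the in-game WebScape.
; On BeginPlay it destroys itself if that URL is already unlocked and starts a timeline that pulses its light.
; Player overlap saves the unlockable after a short delay, shows a message widget with the public name, plays a sound and destroys the pickup.
; It also decrements ItemsLeft on a parent BP_ItemCounter; the per-map URL lookup is noted as unused.
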(event `self.ReceiveBeginPlay`
  (`|ExecutionSequence`
    (:`then_0`
      (if (not (`self.map name independent?`))
        ;[1 1 1] this part isn't actually in use
        (bind _returnvalue (`GameplayStatics.GetCurrentLevelName` true))
        (switch `string` _returnvalue
          (:`Default`
            (set `self.url` "*%$&#^*$&*(%$!!!!!!@"))
          (:`EP2_DOM1`
            (set `self.url` "GalactaMax.com"))
          (:`EP2_DOM2`
            (set `self.url` "Orbital.news"))
          (:`EP2_DOM3`
            (set `self.url` "TheMercenaryBar.net"))
          (:`EP3_CTF1`
            (set `self.url` "TheMercenaryBar.net login"))
          (:`EP3_CTF2`
            (set `self.url` "TeamDecimator.org"))
          (:`EP0_Intro_Tutorial`
            (set `self.url` "TheWizardsLair.com")))))
    (:`then_1`
      (bind _unlocked_ (`/Game/Blueprints/NewFunctionLibrary.has unlockable` (`KismetTextLibrary.Conv_TextToString` (`self.url`))))
      (if _unlocked_
        (`self.K2_DestroyActor`)))
    (:`then_2`
      (bind (_direction _intensity_pulse) (`Timeline|Light` :!via `PlayFromStart`)
        (:`Update`
          (`LightComponent.SetIntensity` (`self.PointLight`) _intensity_pulse))))))

(event `self.Sphere.OnComponentBeginOverlap`
  (params (OverlappedComponent :type "PrimitiveComponent Object Reference") (OtherActor :type "Actor Object Reference") (OtherComp :type "PrimitiveComponent Object Reference") (OtherBodyIndex :type Integer) (bFromSweep :type Boolean) (SweepResult :type "HitResult Structure (by ref)"))
  (cast `/Game/Blueprints/CHARACTERS/fpsMovementCharacter_light_1_vq3` OtherActor)
  (`|ExecutionSequence`
    (:`then_0`
      (`/Engine/EditorBlueprintResources/StandardMacros.DoOnce` false
        (:`Completed`
          (`KismetSystemLibrary.Delay` 0.2)
          (`/Game/Blueprints/NewFunctionLibrary.add unlockable` (`KismetTextLibrary.Conv_TextToString` (`self.url`)))
          (bind _returnvalue (`|CreateWidget` "/Game/Blueprints/UI/UI_Pickups/UI_Pickup_Gen_WebScape.UI_Pickup_Gen_WebScape_C"))
          (set `/Game/Blueprints/UI/UI_Pickups/UI_Pickup_Gen_WebScape.Message` (`KismetTextLibrary.Conv_StringToText` (`KismetStringLibrary.Concat_StrStr` "URL: " (`KismetTextLibrary.Conv_TextToString` (`self.URL_public name`)))) _returnvalue)
          (`UserWidget.AddToViewport` _returnvalue 0)
          (`GameplayStatics.PlaySound2D` "/Game/AUDIO/SFX_Pickups/SC_WeblinkPickup.SC_WeblinkPickup" 1.0 1.0 0.0 null null)
          (`self.K2_DestroyActor`))))
    (:`then_1`
      ;[1 1 1] Calculates values for the Item counter BP
      (bind _asbp_item_counter (cast `/Game/Blueprints/MISC/BP_ItemCounter` (`self.GetParentActor`)))
      (bind _result (`/Engine/EditorBlueprintResources/StandardMacros.DecrementInt` (`/Game/Blueprints/MISC/BP_ItemCounter.Items left` _asbp_item_counter))
        (:`  `
          (set `/Game/Blueprints/MISC/BP_ItemCounter.Items left` _result _asbp_item_counter))))))

(fn `UserConstructionScript`
  (`TextRenderComponent.K2_SetText` (`self.TextRender`) (`self.url`))
  (`TextRenderComponent.K2_SetText` (`self.TextRender1`) (`self.URL_public name`)))