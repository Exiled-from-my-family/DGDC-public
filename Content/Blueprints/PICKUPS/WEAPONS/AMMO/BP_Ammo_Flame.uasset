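; Fuel canister ammo pickup that adds 25 to the player character's LGAmmo, capped at 100, if the player is alive and not full.
; Sphere overlap routes through RocketLauncher-named server and multicast events, with a timed DoOnce limiting repeat triggers.
; Pickup shows a UI message, plays a sound, reports noise and hides the actor.
; When Respawn is set, it reappears after RespawnTime with sound and particles.
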(event `RocketLauncherPickupMulticast`
  (params (Actor :type "Actor Object Reference"))
  (bind _returnvalue (`self.K2_GetActorLocation`))
  ;[0.3687 0.5739 1] Pickup Overlap
  (`|ExecutionSequence`
    (:`then_0`
      (`/Engine/EditorBlueprintResources/StandardMacros.DoOnce` false :!label _label
        (:`Completed`
          (bind _asfps_movement_character_light_1_vq_3 (cast `/Game/Blueprints/CHARACTERS/fpsMovementCharacter_light_1_vq3` Actor))
          (bind _lgammo (`/Game/Blueprints/CHARACTERS/fpsMovementCharacter_light_1_vq3.LGAmmo` _asfps_movement_character_light_1_vq_3))
          (if (and (not (`/Game/Blueprints/CHARACTERS/fpsMovementCharacter_light_1_vq3.IsDead?` _asfps_movement_character_light_1_vq_3)) (< _lgammo 100.0))
            (bind _returnvalue_2 (`|CreateWidget` "/Game/Blueprints/UI/UI_Pickups/UI_Pickup_Gen_Ammo.UI_Pickup_Gen_Ammo_C"))
            (set `/Game/Blueprints/UI/UI_Pickups/UI_Pickup_Gen_Ammo.Message` "Fuel canister (+25)" _returnvalue_2)
            (set `/Game/Blueprints/UI/UI_Pickups/UI_Pickup_Gen_Ammo.Color` (struct :`R` 1.0 :`G` 0.416667 :`A` 1.0) _returnvalue_2)
            (`UserWidget.AddToViewport` _returnvalue_2 0)
            (set `/Game/Blueprints/CHARACTERS/fpsMovementCharacter_light_1_vq3.LGAmmo` (`KismetMathLibrary.FClamp` (+ _lgammo 25.0) 0.0 100.0) _asfps_movement_character_light_1_vq_3)
            (`GameplayStatics.PlaySoundAtLocation` "/Game/AUDIO/SFX_Pickups/SC_AmmoPickup.SC_AmmoPickup" (`self.K2_GetActorLocation`) (struct) 1.0 0.9 0.0 null null null)
            (`AISense_Hearing.ReportNoiseEvent` (`self.K2_GetActorLocation`) 1.0 _asfps_movement_character_light_1_vq_3)
            (`self.SetActorHiddenInGame` true)
            (`self.SetActorEnableCollision` false)
            (`KismetSystemLibrary.Delay` (`self.Respawn Time`))
            (if (`self.respawn?`)
              (`self.SetActorHiddenInGame` false)
              (`self.SetActorEnableCollision` true)
              (`GameplayStatics.PlaySoundAtLocation` "/Game/AUDIO/SFX_Pickups/SC_PickupRespawn.SC_PickupRespawn" _returnvalue (struct) 0.7 1.0 0.0 null null null)
              (`GameplayStatics.SpawnEmitterAtLocation` "/Game/kosm_fps_assets/Misc/Particles/P_LightEmitter1.P_LightEmitter1" (+ _returnvalue (0.0 0.0 50.0)) (struct) (2.5 2.5 2.5)))))))
    (:`then_1`
      (`KismetSystemLibrary.Delay` 1.0)
      (goto _label :!via `Reset`))))

(event `self.Sphere.OnComponentBeginOverlap`
  (params (OverlappedComponent :type "PrimitiveComponent Object Reference") (OtherActor :type "Actor Object Reference") (OtherComp :type "PrimitiveComponent Object Reference") (OtherBodyIndex :type Integer) (bFromSweep :type Boolean) (SweepResult :type "HitResult Structure (by ref)"))
  ;[0.3687 0.5739 1] Pickup Overlap
  (`KismetSystemLibrary.Delay` 0.02)
  (`/Engine/EditorBlueprintResources/ActorMacros.Switch Has Authority`
    (:`Authority`
      (`self.RocketLauncherPickupMulticast` OtherActor))
    (:`Remote`
      (`self.RocketLauncherPickupServer` OtherActor))))

(event `RocketLauncherPickupServer`
  (params (Actor :type "Actor Object Reference"))
  ;[0.3687 0.5739 1] Pickup Overlap
  (`self.RocketLauncherPickupMulticast` Actor))

(fn `UserConstructionScript`)