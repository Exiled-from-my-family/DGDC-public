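; Railgun ("Penetrator") weapon pickup that spins in place and grants railgun ammo, with separate rules for three character classes.
; Overlap routes by authority into events still named RocketLauncherPickup, then plays sound, reports noise, hides the pickup and optionally respawns it with effects.
; Only the vq3 branch registers the unlock and shows the message and one-time announcer; it sets GotRailgun false, while the ep1 branch sets it true.
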(event `RocketLauncherPickupMulticast`
  (params (Actor :type "Actor Object Reference"))
  (bind _returnvalue (`self.K2_GetActorLocation`))
  (bind _returnvalue_2 (`self.K2_GetActorLocation`))
  ;[0.3687 0.5739 1] Pickup Overlap
  (bind _asfps_movement_character_light_1_vq_3 (cast `/Game/Blueprints/CHARACTERS/fpsMovementCharacter_light_1_vq3` Actor)
    (:`then`
      (set `/Game/Blueprints/CHARACTERS/fpsMovementCharacter_light_1_vq3.Got_Railgun` false _asfps_movement_character_light_1_vq_3)
      (`/Game/Blueprints/NewFunctionLibrary.add unlockable` "RAILGUN")
      (`/Game/Blueprints/NewFunctionLibrary.clean all message widgets`)
      (`KismetSystemLibrary.Delay` 0.01)
      (bind _returnvalue_3 (`|CreateWidget` "/Game/Blueprints/UI/UI_Pickups/UI_Pickup_Gen_Weapon.UI_Pickup_Gen_Weapon_C"))
      (set `/Game/Blueprints/UI/UI_Pickups/UI_Pickup_Gen_Weapon.Message` "Penetrator" _returnvalue_3)
      (`UserWidget.AddToViewport` _returnvalue_3 0)
      (set `/Game/Blueprints/CHARACTERS/fpsMovementCharacter_light_1_vq3.RailgunAmmo` (`KismetMathLibrary.Clamp` (+ (`/Game/Blueprints/CHARACTERS/fpsMovementCharacter_light_1_vq3.RailgunAmmo` _asfps_movement_character_light_1_vq_3) 6) 0 10) _asfps_movement_character_light_1_vq_3)
      (`GameplayStatics.PlaySoundAtLocation` "/Game/AUDIO/SFX_Pickups/SC_WeaponPickup.SC_WeaponPickup" _returnvalue (struct) 1.0 1.0 0.0 null null null)
      (`|ExecutionSequence`
        (:`then_0`
          (`AISense_Hearing.ReportNoiseEvent` (`self.K2_GetActorLocation`) 1.0 _asfps_movement_character_light_1_vq_3)
          (`self.SetActorHiddenInGame` true :!label _label)
          (`self.SetActorEnableCollision` false)
          (`KismetSystemLibrary.Delay` (`self.respawn time`))
          (if (`self.respawn?`)
            (`self.SetActorHiddenInGame` false)
            (`self.SetActorEnableCollision` true)
            (`GameplayStatics.PlaySoundAtLocation` "/Game/AUDIO/SFX_Pickups/SC_PickupRespawn.SC_PickupRespawn" _returnvalue_2 (struct) 0.7 1.0 0.0 null null null)
            (`GameplayStatics.SpawnEmitterAtLocation` "/Game/kosm_fps_assets/Misc/Particles/P_LightEmitter1.P_LightEmitter1" (+ _returnvalue_2 (0.0 0.0 75.0)) (struct) (3.0 3.0 3.0))))
        (:`then_1`
          (`KismetSystemLibrary.Delay` 0.3)
          (`/Engine/EditorBlueprintResources/StandardMacros.DoOnce` false
            (:`Completed`
              (`GameplayStatics.PlaySound2D` (`self.Announcer Weapon`) 1.0 1.0 0.0 null null))))))
    (:`CastFailed`
      (bind _asfps_movement_character_light_2_cpma (cast `/Game/Blueprints/CHARACTERS/fpsMovementCharacter_light_2_cpma` Actor)
        (:`then`
          (bind _railgunammo (`/Game/Blueprints/CHARACTERS/fpsMovementCharacter_light_2_cpma.RailgunAmmo` _asfps_movement_character_light_2_cpma))
          (if (< _railgunammo 10)
            (set `/Game/Blueprints/CHARACTERS/fpsMovementCharacter_light_2_cpma.RailgunAmmo` 10 _asfps_movement_character_light_2_cpma)
            (`GameplayStatics.PlaySoundAtLocation` "/Game/AUDIO/SFX_Pickups/SC_WeaponPickup.SC_WeaponPickup" _returnvalue (struct) 1.0 1.0 0.0 null null null :!label _label_2)
            (`AISense_Hearing.ReportNoiseEvent` (`self.K2_GetActorLocation`) 1.0 _asfps_movement_character_light_2_cpma)
            (goto _label)
            (elif (not (>= _railgunammo 25))
              (set `/Game/Blueprints/CHARACTERS/fpsMovementCharacter_light_2_cpma.RailgunAmmo` (`KismetMathLibrary.Clamp` (+ _railgunammo 1) 0 25) _asfps_movement_character_light_2_cpma)
              (goto _label_2))))
        (:`CastFailed`
          (bind _asep_1_character (cast `/Game/MISSIONS/EP1/Characters/ep1_character` Actor))
          (set `/Game/MISSIONS/EP1/Characters/ep1_character.got_railgun` true _asep_1_character)
          (set `/Game/MISSIONS/EP1/Characters/ep1_character.Ammo_Railgun` (`KismetMathLibrary.Clamp` (+ (`/Game/MISSIONS/EP1/Characters/ep1_character.Ammo_Railgun` _asep_1_character) 3) 0 10) _asep_1_character)
          (goto _label_2))))))

(event `self.ReceiveActorBeginOverlap`
  (params (OtherActor :type "Actor Object Reference"))
  ;[0.3687 0.5739 1] Pickup Overlap
  (`KismetSystemLibrary.Delay` 0.02)
  (`/Engine/EditorBlueprintResources/ActorMacros.Switch Has Authority`
    (:`Authority`
      (`self.RocketLauncherPickupMulticast` OtherActor))
    (:`Remote`
      (`self.RocketLauncherPickupServer` OtherActor))))

(event `self.ReceiveTick`
  (params (DeltaSeconds :type "Float (single-precision)"))
  ;[0.3687 0.5739 1] Pickup Overlap
  ;;[1 1 1] NEW ROTATION COMPONENT: FLOAT VALUE DEFINES ROTATION SPEED, ELIMINATED VETICAL FLOATING
  (`self.K2_AddActorLocalRotation` (`KismetMathLibrary.MakeRotator` 0.0 0.0 (* DeltaSeconds 45.0))))

(event `RocketLauncherPickupServer`
  (params (Actor :type "Actor Object Reference"))
  ;[0.3687 0.5739 1] Pickup Overlap
  (`self.RocketLauncherPickupMulticast` Actor))

(fn `UserConstructionScript`)