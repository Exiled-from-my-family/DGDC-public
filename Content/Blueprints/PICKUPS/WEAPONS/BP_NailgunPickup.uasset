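; Spinning Nailgun pickup that reacts to overlap through authority-switched server and multicast events still named after the rocket launcher.
; For the vq3 character it switches to the Nailgun, shows a pickup message and HUD elements, then destroys itself.
; For the cpma character it tops up or increments capped ammo, reports noise, then hides and respawns after a short delay.
; Alternate vq3 ammo and respawn logic is left disconnected.
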(event `RocketLauncherPickupMulticast`
  (params (Actor :type "Actor Object Reference"))
  (bind _returnvalue (`self.K2_GetActorLocation`))
  ;[0.3687 0.5739 1] Pickup Overlap
  (bind _asfps_movement_character_light_1_vq_3 (cast `/Game/Blueprints/CHARACTERS/fpsMovementCharacter_light_1_vq3` Actor)
    (:`then`
      (`/Game/Blueprints/CHARACTERS/fpsMovementCharacter_light_1_vq3.Switch nailgun` _asfps_movement_character_light_1_vq_3)
      (`SceneComponent.SetVisibility` (`/Game/Blueprints/CHARACTERS/fpsMovementCharacter_light_1_vq3.1PGun` _asfps_movement_character_light_1_vq_3) true false)
      (set `/Game/Blueprints/CHARACTERS/fpsMovementCharacter_light_1_vq3.bad template no weapon scroll` 0 _asfps_movement_character_light_1_vq_3)
      (`/Game/Blueprints/CHARACTERS/fpsMovementCharacter_light_1_vq3.SwitchAnim` _asfps_movement_character_light_1_vq_3)
      (set `/Game/Blueprints/CHARACTERS/fpsMovementCharacter_light_1_vq3.WeaponSwitch?` false _asfps_movement_character_light_1_vq_3)
      (`/Game/Blueprints/NewFunctionLibrary.clean all message widgets`)
      (`KismetSystemLibrary.Delay` 0.01)
      (bind _returnvalue_2 (`|CreateWidget` "/Game/Blueprints/UI/UI_Pickups/UI_Pickup_Gen_Weapon.UI_Pickup_Gen_Weapon_C"))
      (set `/Game/Blueprints/UI/UI_Pickups/UI_Pickup_Gen_Weapon.Message` "Nailgun" _returnvalue_2)
      (bind _player (`/Game/Blueprints/NewFunctionLibrary.get player`))
      (`Widget.SetVisibility` (`/Game/Blueprints/UI/HUD_vq3.Nailgun_ICON` (`/Game/Blueprints/CHARACTERS/fpsMovementCharacter_light_1_vq3.HUD` _player)) "Visible")
      (`Widget.SetVisibility` (`/Game/Blueprints/UI/HUD_vq3.NailgunAmmo` (`/Game/Blueprints/CHARACTERS/fpsMovementCharacter_light_1_vq3.HUD` _player)) "Visible")
      (`Widget.SetVisibility` (`/Game/Blueprints/UI/HUD_vq3.Hud_piece_2` (`/Game/Blueprints/CHARACTERS/fpsMovementCharacter_light_1_vq3.HUD` _player)) "Visible")
      (`GameplayStatics.PlaySoundAtLocation` "/Game/AUDIO/SFX_Pickups/SC_WeaponPickup.SC_WeaponPickup" _returnvalue (struct) 1.0 1.0 0.0 null null null)
      (`self.K2_DestroyActor`))
    (:`CastFailed`
      (bind _asfps_movement_character_light_2_cpma (cast `/Game/Blueprints/CHARACTERS/fpsMovementCharacter_light_2_cpma` Actor))
      (bind _nailgunammo (`/Game/Blueprints/CHARACTERS/fpsMovementCharacter_light_2_cpma.NailgunAmmo` _asfps_movement_character_light_2_cpma))
      (if (< _nailgunammo 100)
        (set `/Game/Blueprints/CHARACTERS/fpsMovementCharacter_light_2_cpma.NailgunAmmo` 100 _asfps_movement_character_light_2_cpma)
        (`GameplayStatics.PlaySoundAtLocation` "/Game/AUDIO/SFX_Pickups/SC_WeaponPickup.SC_WeaponPickup" _returnvalue (struct) 1.0 1.0 0.0 null null null :!label _label)
        (`AISense_Hearing.ReportNoiseEvent` (`self.K2_GetActorLocation`) 1.0 _asfps_movement_character_light_2_cpma)
        (`self.SetActorHiddenInGame` true)
        (`self.SetActorEnableCollision` false)
        (`KismetSystemLibrary.Delay` 1.0)
        (`self.SetActorHiddenInGame` false)
        (`self.SetActorEnableCollision` true)
        (`GameplayStatics.PlaySoundAtLocation` "/Game/AUDIO/SFX_Pickups/SC_PickupRespawn.SC_PickupRespawn" (`self.K2_GetActorLocation`) (struct) 0.7 1.0 0.0 null null null)
        (elif (not (>= _nailgunammo 150))
          (set `/Game/Blueprints/CHARACTERS/fpsMovementCharacter_light_2_cpma.NailgunAmmo` (`KismetMathLibrary.Clamp` (+ _nailgunammo 10) 0 150) _asfps_movement_character_light_2_cpma)
          (goto _label))))))

(event `self.ReceiveActorBeginOverlap`
  (params (OtherActor :type "Actor Object Reference"))
  ;[0.3687 0.5739 1] Pickup Overlap
  (`KismetSystemLibrary.Delay` 0.02)
  (`/Engine/EditorBlueprintResources/ActorMacros.Switch Has Authority`
    (:`Authority`
      (`self.RocketLauncherPickupMulticast` OtherActor))
    (:`Remote`
      (`self.RocketLauncherPickupServer` OtherActor))))

(event `self.ReceiveTick`
  (params (DeltaSeconds :type "Float (single-precision)"))
  ;[0.3687 0.5739 1] Pickup Overlap
  ;;[1 1 1] NEW ROTATION COMPONENT: FLOAT VALUE DEFINES ROTATION SPEED, ELIMINATED VETICAL FLOATING
  (`self.K2_AddActorLocalRotation` (`KismetMathLibrary.MakeRotator` 0.0 0.0 (* DeltaSeconds 45.0))))

(event `RocketLauncherPickupServer`
  (params (Actor :type "Actor Object Reference"))
  ;[0.3687 0.5739 1] Pickup Overlap
  (`self.RocketLauncherPickupMulticast` Actor))

(fn `UserConstructionScript`)