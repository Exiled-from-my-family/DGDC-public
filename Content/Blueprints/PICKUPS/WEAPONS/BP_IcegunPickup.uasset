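; Ice cannon weapon pickup that grants a weapon slot and ammo to a living player character on overlap.
; Overlap routes by authority through events named for the rocket launcher, while the weapon itself reuses the character's grenade launcher ammo and switch logic.
; It shows a pickup message, plays sound, reports noise, then hides and optionally respawns after a delay with effects.
; A first-time pickup also shows a tutorial, gated by the "first_ice" unlockable.
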(event `RocketLauncherPickupMulticast`
  (params (Actor :type "Actor Object Reference"))
  (bind _returnvalue (`self.K2_GetActorLocation`))
  ;[0.3687 0.5739 1] Pickup Overlap
  (bind _asfps_movement_character_light_1_vq_3 (cast `/Game/Blueprints/CHARACTERS/fpsMovementCharacter_light_1_vq3` Actor))
  (if (not (`/Game/Blueprints/CHARACTERS/fpsMovementCharacter_light_1_vq3.IsDead?` _asfps_movement_character_light_1_vq_3))
    (`BlueprintMapLibrary.Map_Add` (`/Game/Blueprints/CHARACTERS/fpsMovementCharacter_light_1_vq3.WeaponSlotIndex` _asfps_movement_character_light_1_vq_3) 2 (`KismetMathLibrary.Clamp` 1 1 1))
    (`/Game/Blueprints/NewFunctionLibrary.clean all message widgets`)
    (`WidgetSwitcher.SetActiveWidgetIndex` (`/Game/Blueprints/UI/HUD_vq3.WidgetSwitcher_GL` (`/Game/Blueprints/CHARACTERS/fpsMovementCharacter_light_1_vq3.HUD` _asfps_movement_character_light_1_vq_3)) 1)
    (bind _returnvalue_2 (`|CreateWidget` "/Game/Blueprints/UI/UI_Pickups/UI_Pickup_Gen_Weapon.UI_Pickup_Gen_Weapon_C"))
    (set `/Game/Blueprints/UI/UI_Pickups/UI_Pickup_Gen_Weapon.Message` "Ice cannon" _returnvalue_2)
    (`UserWidget.AddToViewport` _returnvalue_2 0)
    (set `/Game/Blueprints/CHARACTERS/fpsMovementCharacter_light_1_vq3.GrenadeLauncherAmmo` (`KismetMathLibrary.Clamp` (+ (`/Game/Blueprints/CHARACTERS/fpsMovementCharacter_light_1_vq3.GrenadeLauncherAmmo` _asfps_movement_character_light_1_vq_3) 14) 0 32) _asfps_movement_character_light_1_vq_3)
    (if (`/Game/Blueprints/CHARACTERS/fpsMovementCharacter_light_1_vq3.Got_GrenadeLauncher` _asfps_movement_character_light_1_vq_3)
      (set `/Game/Blueprints/CHARACTERS/fpsMovementCharacter_light_1_vq3.Got_GrenadeLauncher` false _asfps_movement_character_light_1_vq_3)
      (`/Game/Blueprints/CHARACTERS/fpsMovementCharacter_light_1_vq3.Switch grenade launcher` _asfps_movement_character_light_1_vq_3))
    (`GameplayStatics.PlaySoundAtLocation` "/Game/AUDIO/SFX_Pickups/SC_WeaponPickup.SC_WeaponPickup" (`self.K2_GetActorLocation`) (struct) 1.0 1.0 0.0 null null null)
    (`AISense_Hearing.ReportNoiseEvent` (`self.K2_GetActorLocation`) 1.0 _asfps_movement_character_light_1_vq_3)
    (`|ExecutionSequence`
      (:`then_0`
        (`self.SetActorHiddenInGame` true)
        (`self.SetActorEnableCollision` false)
        (`KismetSystemLibrary.Delay` (`self.Respawn Time`))
        (if (`self.respawn?`)
          (`self.SetActorHiddenInGame` false)
          (`self.SetActorEnableCollision` true)
          (`GameplayStatics.PlaySoundAtLocation` "/Game/AUDIO/SFX_Pickups/SC_PickupRespawn.SC_PickupRespawn" _returnvalue (struct) 0.7 1.0 0.0 null null null)
          (`GameplayStatics.SpawnEmitterAtLocation` "/Game/kosm_fps_assets/Misc/Particles/P_LightEmitter1.P_LightEmitter1" (+ _returnvalue (0.0 0.0 75.0)) (struct) (3.0 3.0 3.0))))
      (:`then_1`
        (bind _unlocked_ (`/Game/Blueprints/NewFunctionLibrary.has unlockable` "first_ice"))
        (if (not _unlocked_)
          (bind _returnvalue_3 (`|CreateWidget` "/Game/Blueprints/UI/UI_PauseTutorials/W_PauseTutorialGeneric_small_noinputs.W_PauseTutorialGeneric_small_noinputs_C" null "PRIMARY: ice pellets that deal damage over time \nSECONDARY: ice bomb. freezes enemies in its radius"))
          (`UserWidget.AddToViewport` _returnvalue_3 0)
          (`/Game/Blueprints/NewFunctionLibrary.add unlockable` "first_ice"))))))

(event `self.ReceiveActorBeginOverlap`
  (params (OtherActor :type "Actor Object Reference"))
  ;[0.3687 0.5739 1] Pickup Overlap
  (`KismetSystemLibrary.Delay` 0.02)
  (`/Engine/EditorBlueprintResources/ActorMacros.Switch Has Authority`
    (:`Authority`
      (`self.RocketLauncherPickupMulticast` OtherActor))
    (:`Remote`
      (`self.RocketLauncherPickupServer` OtherActor))))

(event `self.ReceiveTick`
  (params (DeltaSeconds :type "Float (single-precision)"))
  ;[0.3687 0.5739 1] Pickup Overlap
  ;;[1 1 1] NEW ROTATION COMPONENT: FLOAT VALUE DEFINES ROTATION SPEED, ELIMINATED VETICAL FLOATING
)

(event `RocketLauncherPickupServer`
  (params (Actor :type "Actor Object Reference"))
  ;[0.3687 0.5739 1] Pickup Overlap
  (`self.RocketLauncherPickupMulticast` Actor))

(fn `UserConstructionScript`)