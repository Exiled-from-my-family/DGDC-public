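; Spinning grenade launcher pickup that grants the weapon or capped ammo to living player characters or eligible ep1_characters (not Robot or Ghost).
; Overlaps route by authority through RocketLauncher-named server and multicast events, which apply the pickup.
; Player pickups show a message and play an announcer line, then flag all instances as announced.
; Collection reports noise and hides the actor, which reappears with effects after RespawnTime if Respawn is set.
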(event `RocketLauncherPickupMulticast`
  (params (Actor :type "Actor Object Reference"))
  (bind _returnvalue (`self.K2_GetActorLocation`))
  ;[0.3687 0.5739 1] Pickup Overlap
  (bind _asfps_movement_character_light_1_vq_3 (cast `/Game/Blueprints/CHARACTERS/fpsMovementCharacter_light_1_vq3` Actor)
    (:`then`
      (if (not (`/Game/Blueprints/CHARACTERS/fpsMovementCharacter_light_1_vq3.IsDead?` _asfps_movement_character_light_1_vq_3))
        (`/Game/Blueprints/NewFunctionLibrary.clean all message widgets`)
        (`KismetSystemLibrary.Delay` 0.05)
        (`/Engine/EditorBlueprintResources/StandardMacros.IsValid` _asfps_movement_character_light_1_vq_3
          (:`Is Valid`
            (bind _returnvalue_2 (`|CreateWidget` "/Game/Blueprints/UI/UI_Pickups/UI_Pickup_Gen_Weapon.UI_Pickup_Gen_Weapon_C"))
            (set `/Game/Blueprints/UI/UI_Pickups/UI_Pickup_Gen_Weapon.Message` "Grenade Launcher" _returnvalue_2)
            (`UserWidget.AddToViewport` _returnvalue_2 0)
            (set `/Game/Blueprints/CHARACTERS/fpsMovementCharacter_light_1_vq3.GrenadeLauncherAmmo` (`KismetMathLibrary.Clamp` (+ (`/Game/Blueprints/CHARACTERS/fpsMovementCharacter_light_1_vq3.GrenadeLauncherAmmo` _asfps_movement_character_light_1_vq_3) 3) 0 9) _asfps_movement_character_light_1_vq_3)
            (if (`/Game/Blueprints/CHARACTERS/fpsMovementCharacter_light_1_vq3.Got_GrenadeLauncher` _asfps_movement_character_light_1_vq_3)
              (set `/Game/Blueprints/CHARACTERS/fpsMovementCharacter_light_1_vq3.Got_GrenadeLauncher` false _asfps_movement_character_light_1_vq_3)
              (`/Game/Blueprints/CHARACTERS/fpsMovementCharacter_light_1_vq3.Switch grenade launcher` _asfps_movement_character_light_1_vq_3))
            (`GameplayStatics.PlaySoundAtLocation` "/Game/AUDIO/SFX_Pickups/SC_WeaponPickup.SC_WeaponPickup" (`self.K2_GetActorLocation`) (struct) 1.0 1.0 0.0 null null null)
            (`|ExecutionSequence`
              (:`then_0`
                (`AISense_Hearing.ReportNoiseEvent` (`self.K2_GetActorLocation`) 1.0 _asfps_movement_character_light_1_vq_3 :!label _label)
                (`self.SetActorHiddenInGame` true)
                (`self.SetActorEnableCollision` false)
                (`KismetSystemLibrary.Delay` (`self.Respawn Time`))
                (if (`self.respawn?`)
                  (`self.SetActorHiddenInGame` false)
                  (`self.SetActorEnableCollision` true)
                  (`GameplayStatics.PlaySoundAtLocation` "/Game/AUDIO/SFX_Pickups/SC_PickupRespawn.SC_PickupRespawn" _returnvalue (struct) 0.7 1.0 0.0 null null null)
                  (`GameplayStatics.SpawnEmitterAtLocation` "/Game/kosm_fps_assets/Misc/Particles/P_LightEmitter1.P_LightEmitter1" (+ _returnvalue (0.0 0.0 75.0)) (struct) (3.0 3.0 3.0))))
              (:`then_1`
                (if (not (`self.Announced?`))
                  (`KismetSystemLibrary.Delay` 0.25)
                  (`/Engine/EditorBlueprintResources/StandardMacros.DoOnce` false
                    (:`Completed`
                      (`GameplayStatics.PlaySound2D` (`self.Announcer Weapon`) 1.0 1.0 0.0 null null)
                      (bind _outactors (`GameplayStatics.GetAllActorsOfClass` "BP_GrenadeLauncherPickup_C"))
                      (for (_ _array_index) _outactors
                        (set `/Game/Blueprints/PICKUPS/WEAPONS/BP_GrenadeLauncherPickup.Announced?` true (`|GetArrayItem` _outactors _array_index))))))))))))
    (:`CastFailed`
      (bind _asep_1_character (cast `/Game/MISSIONS/EP1/Characters/ep1_character` Actor))
      (if (not (or (`/Game/Blueprints/CHARACTERS/NoobotAI/Blueprints/AI_NoobotChar.IsDead?` _asep_1_character) (`self.ActorHasTag` _asep_1_character "Robot") (`self.ActorHasTag` _asep_1_character "Ghost")))
        (set `/Game/MISSIONS/EP1/Characters/ep1_character.gotcha_grenade` true _asep_1_character)
        (set `/Game/MISSIONS/EP1/Characters/ep1_character.Ammo_Grenade` (`KismetMathLibrary.Clamp` (+ (`/Game/MISSIONS/EP1/Characters/ep1_character.Ammo_Grenade` _asep_1_character) 3) 0 9) _asep_1_character)
        (`GameplayStatics.PlaySoundAtLocation` "/Game/AUDIO/SFX_Pickups/SC_WeaponPickup.SC_WeaponPickup" (`self.K2_GetActorLocation`) (struct) 1.0 1.0 0.0 null null null)
        (goto _label)))))

(event `self.ReceiveActorBeginOverlap`
  (params (OtherActor :type "Actor Object Reference"))
  ;[0.3687 0.5739 1] Pickup Overlap
  (`KismetSystemLibrary.Delay` 0.02)
  (`/Engine/EditorBlueprintResources/ActorMacros.Switch Has Authority`
    (:`Authority`
      (`self.RocketLauncherPickupMulticast` OtherActor))
    (:`Remote`
      (`self.RocketLauncherPickupServer` OtherActor))))

(event `self.ReceiveTick`
  (params (DeltaSeconds :type "Float (single-precision)"))
  ;[0.3687 0.5739 1] Pickup Overlap
  ;;[1 1 1] NEW ROTATION COMPONENT: FLOAT VALUE DEFINES ROTATION SPEED, ELIMINATED VETICAL FLOATING
  (`self.K2_AddActorLocalRotation` (`KismetMathLibrary.MakeRotator` 0.0 0.0 (* DeltaSeconds (`self.Rotation`)))))

(event `RocketLauncherPickupServer`
  (params (Actor :type "Actor Object Reference"))
  ;[0.3687 0.5739 1] Pickup Overlap
  (`self.RocketLauncherPickupMulticast` Actor))

(fn `UserConstructionScript`)