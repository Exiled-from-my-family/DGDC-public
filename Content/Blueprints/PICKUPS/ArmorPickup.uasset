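; Armor pickup that grants a capped armor boost to the two light FPS movement character types (VQ3 and CPMA) when they overlap it.
; Overlap routes by authority through server and multicast-named events, which update armor and its 3D widget bar, play a sound and report noise.
; A successful pickup hides the actor and disables collision, then respawns it with a sound after a delay.
; A rotation and movement timeline exists but never runs.
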(event `self.ReceiveActorBeginOverlap`
  (params (OtherActor :type "Actor Object Reference"))
  ;[0.3687 0.5739 1] Pickup Overlap
  (`/Engine/EditorBlueprintResources/ActorMacros.Switch Has Authority`
    (:`Authority`
      (`self.ArmorPickupMulticast` OtherActor))
    (:`Remote`
      (`self.ArmorPickupServer` OtherActor))))

(event `ArmorPickupMulticast`
  (params (Actor :type "Actor Object Reference"))
  (bind _returnvalue (`self.K2_GetActorLocation`))
  ;[0.3687 0.5739 1] Pickup Overlap
  (bind _asfps_movement_character_light_1_vq_3 (cast `/Game/Blueprints/CHARACTERS/fpsMovementCharacter_light_1_vq3` Actor)
    (:`then`
      (bind _armor (`/Game/Blueprints/CHARACTERS/fpsMovementCharacter_light_1_vq3.Armor` _asfps_movement_character_light_1_vq_3))
      (if (not (>= _armor 50.0))
        (bind _output_get (set `/Game/Blueprints/CHARACTERS/fpsMovementCharacter_light_1_vq3.Armor` (`KismetMathLibrary.FClamp` (+ _armor 15.0) 0.0 50.0) _asfps_movement_character_light_1_vq_3))
        (message `/Game/Blueprints/UI/UI_Interface.SetArmorBarPercent` (`WidgetComponent.GetUserWidgetObject` (`/Game/Blueprints/CHARACTERS/fpsMovementCharacter_light_1_vq3.HealthBar_3D_WG` _asfps_movement_character_light_1_vq_3)) (/ _output_get 100.0))
        (`GameplayStatics.PlaySoundAtLocation` "/Game/AUDIO/SFX_Pickups/SC_ArmorPickup.SC_ArmorPickup" _returnvalue (struct) 0.4 1.0 0.0 null null null)
        (`AISense_Hearing.ReportNoiseEvent` (`self.K2_GetActorLocation`) 1.0 _asfps_movement_character_light_1_vq_3)
        (`self.SetActorHiddenInGame` true :!label _label)
        (`self.SetActorEnableCollision` false)
        (`KismetSystemLibrary.Delay` 30.0)
        (`self.SetActorHiddenInGame` false)
        (`self.SetActorEnableCollision` true)
        (`GameplayStatics.PlaySoundAtLocation` "/Game/AUDIO/SFX_Pickups/SC_PickupRespawn.SC_PickupRespawn" (`self.K2_GetActorLocation`) (struct) 0.7 1.0 0.0 null null null)))
    (:`CastFailed`
      (bind _asfps_movement_character_light_2_cpma (cast `/Game/Blueprints/CHARACTERS/fpsMovementCharacter_light_2_cpma` Actor))
      (bind _armor_2 (`/Game/Blueprints/CHARACTERS/fpsMovementCharacter_light_2_cpma.Armor` _asfps_movement_character_light_2_cpma))
      (if (not (>= _armor_2 50.0))
        (bind _output_get_2 (set `/Game/Blueprints/CHARACTERS/fpsMovementCharacter_light_2_cpma.Armor` (`KismetMathLibrary.FClamp` (+ _armor_2 15.0) 0.0 50.0) _asfps_movement_character_light_2_cpma))
        (message `/Game/Blueprints/UI/UI_Interface.SetArmorBarPercent` (`WidgetComponent.GetUserWidgetObject` (`/Game/Blueprints/CHARACTERS/fpsMovementCharacter_light_2_cpma.HealthBar_3D_WG` _asfps_movement_character_light_2_cpma)) (/ _output_get_2 100.0))
        (`GameplayStatics.PlaySoundAtLocation` "/Game/AUDIO/SFX_Pickups/SC_ArmorPickup.SC_ArmorPickup" _returnvalue (struct) 0.4 1.0 0.0 null null null)
        (`AISense_Hearing.ReportNoiseEvent` (`self.K2_GetActorLocation`) 1.0 _asfps_movement_character_light_2_cpma)
        (goto _label)))))

(event `ArmorPickupServer`
  (params (Actor :type "Actor Object Reference"))
  ;[0.3687 0.5739 1] Pickup Overlap
  (`self.ArmorPickupMulticast` Actor))

(fn `UserConstructionScript`)