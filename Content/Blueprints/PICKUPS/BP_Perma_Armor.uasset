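; BP_Perma_Armor is a spinning Enduring Armor shard pickup that permanently raises the player's starting armor.
; On player overlap it adds Amount to the game instance's StartArmor, records an unlock and shows a pickup message, plus a tutorial for the first shard.
; Unlock IDs combine level and object name unless CustomId is set, so collected or disabled shards self-destroy on BeginPlay.
; The construction script counts enabled shards in the level.
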(event `self.ReceiveTick`
  (params (DeltaSeconds :type "Float (single-precision)"))
  (`SceneComponent.K2_AddLocalRotation` (`self.armor_shard`) (`KismetMathLibrary.MakeRotator` 0.0 0.0 (* DeltaSeconds 45.0)) false false))

(event `self.ReceiveBeginPlay`
  (bind _game_instance (`/Game/Blueprints/NewFunctionLibrary.dead game instance`))
  (bind _returnvalue (`self.unlock name`))
  (bind _unlocks (`/Game/Blueprints/DeadGaemInstance.unlocks` _game_instance))
  (if (`BlueprintSetLibrary.Set_Contains` _unlocks _returnvalue)
    (`self.K2_DestroyActor` :!label _label)
    (else
      (bind _returnvalue_2 (`self.unlock name_A`))
      (if (`BlueprintSetLibrary.Set_Contains` _unlocks _returnvalue_2)
        (goto _label)
        (elif (`self.disabled/not for this playthrough`)
          (goto _label))))))

(event `self.armor_shard.OnComponentBeginOverlap`
  (params (OverlappedComponent :type "PrimitiveComponent Object Reference") (OtherActor :type "Actor Object Reference") (OtherComp :type "PrimitiveComponent Object Reference") (OtherBodyIndex :type Integer) (bFromSweep :type Boolean) (SweepResult :type "HitResult Structure (by ref)"))
  (cast `/Game/Blueprints/CHARACTERS/fpsMovementCharacter_light_1_vq3` OtherActor)
  (`/Engine/EditorBlueprintResources/StandardMacros.DoOnce` false
    (:`Completed`
      (`AudioComponent.Stop` (`self.Ambient loop`))
      (bind _returnvalue (`|CreateWidget` "/Game/Blueprints/UI/UI_Pickups/UI_Pickup_Gen_Ammo.UI_Pickup_Gen_Ammo_C"))
      (set `/Game/Blueprints/UI/UI_Pickups/UI_Pickup_Gen_Ammo.Message` (`KismetTextLibrary.Conv_StringToText` (`KismetStringLibrary.Concat_StrStr` "Enduring Armor Shard (+" (`KismetStringLibrary.Conv_IntToString` (`self.amount`)) ")")) _returnvalue)
      (set `/Game/Blueprints/UI/UI_Pickups/UI_Pickup_Gen_Ammo.Color` (struct :`R` 0.706331 :`G` 1.0 :`B` 0.932563 :`A` 1.0) _returnvalue)
      (`UserWidget.AddToViewport` _returnvalue 0)
      (bind _game_instance (`/Game/Blueprints/NewFunctionLibrary.dead game instance`))
      (if (== (`/Game/Blueprints/DeadGaemInstance.Start Armor` _game_instance) 0)
        (if (`self.not debug`)
          (`self.Pick item`)
          (`KismetSystemLibrary.Delay` 1.0)
          (bind _returnvalue_2 (`|CreateWidget` "/Game/Blueprints/UI/UI_PauseTutorials/W_PauseTutorialGeneric.W_PauseTutorialGeneric_C"))
          (set `/Game/Blueprints/UI/UI_PauseTutorials/W_PauseTutorialGeneric.Message` "This is a shard of Enduring Armor. \n \nThis armor set permantly regenerates armor as long as you have less than 5 armor for each shard." _returnvalue_2)
          (`UserWidget.AddToViewport` _returnvalue_2 0)
          (else
            (bind _game_instance_2 (`/Game/Blueprints/NewFunctionLibrary.dead game instance` :!label _label_2))
            (bind _returnvalue_3 (`self.unlock name`))
            (`KismetSystemLibrary.PrintString` _returnvalue_3 true false (struct :`G` 0.66 :`B` 1.0 :`A` 1.0) 10.0)
            (`BlueprintSetLibrary.Set_Add` (`/Game/Blueprints/DeadGaemInstance.unlocks` _game_instance_2) _returnvalue_3)
            (bind _output_get (set `/Game/Blueprints/DeadGaemInstance.Start Armor` (+ (`/Game/Blueprints/DeadGaemInstance.Start Armor` _game_instance_2) (`self.amount`)) _game_instance_2))
            (bind _player (`/Game/Blueprints/NewFunctionLibrary.get player`))
            (set `/Game/Blueprints/CHARACTERS/fpsMovementCharacter_light_1_vq3.start armor for map` _output_get _player)
            (`GameplayStatics.PlaySound2D` "/Game/AUDIO/SFX_Pickups/SW_Armor100.SW_Armor100" 1.0 1.5 0.0 null null)
            (`GameplayStatics.PlaySound2D` "/Game/AUDIO/portalthrough2.portalthrough2" 1.0 2.0 0.0 null null)
            (`SceneComponent.ToggleVisibility` (`self.DefaultSceneRoot`) true)
            (`KismetSystemLibrary.Delay` 1.5)
            (`self.K2_DestroyActor`)))
        (else
          (goto _label_2))))))

(event `Pick item`
  (`/Engine/EditorBlueprintResources/StandardMacros.DoOnce` false
    (:`Completed`
      (goto _label_2))))

(fn `UserConstructionScript`
  (`SceneComponent.SetVisibility` (`self.PointLight`) (`self.not debug`) false)
  (`SceneComponent.SetVisibility` (`self.Niagara`) (`self.not debug`) false)
  (bind _outactors (`GameplayStatics.GetAllActorsOfClass` "BP_Perma_Armor_C"))
  (set `self.number of total shards in level` 0)
  (for _array_element _outactors
    (if (not (`/Game/Blueprints/PICKUPS/BP_Perma_Armor.disabled/not for this playthrough` _array_element))
      (`/Engine/EditorBlueprintResources/StandardMacros.IncrementInt` (`self.number of total shards in level`))))
  (if (`self.Custom id`)
    ;[1 1 1] this was to keep the original unlockables used in EP1
    (set `self.object id` (`self.object id`))
    (else
      (set `self.object id` (`KismetSystemLibrary.GetObjectName` self)))))