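; Bubble gun projectile that bursts with radial damage, a physics impulse, particles, sound and camera shake.
; It detonates on a short BeginPlay fuse with the strongest blast, on overlapping a non-instigator, or after limited bounces.
; A hit on non-movable geometry also triggers a delayed burst with a bullet-hole decal, though the fuse is far shorter.
; Tick billboards StaticMesh1 toward the first player's pawn.
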(event `self.ReceiveTick`
  (params (DeltaSeconds :type "Float (single-precision)"))
  (bind _staticmesh1 (`self.StaticMesh1`))
  (`SceneComponent.K2_SetWorldRotation` _staticmesh1 (`KismetMathLibrary.MakeRotator` (.roll (`KismetMathLibrary.FindLookAtRotation` (`SceneComponent.K2_GetComponentLocation` _staticmesh1) (`self.K2_GetActorLocation` (`GameplayStatics.GetPlayerPawn` 0)))) (- (.pitch (`KismetMathLibrary.FindLookAtRotation` (`SceneComponent.K2_GetComponentLocation` _staticmesh1) (`self.K2_GetActorLocation` (`GameplayStatics.GetPlayerPawn` 0)))) 90.0) (.yaw (`KismetMathLibrary.FindLookAtRotation` (`SceneComponent.K2_GetComponentLocation` _staticmesh1) (`self.K2_GetActorLocation` (`GameplayStatics.GetPlayerPawn` 0))))) false false))

(event `self.ReceiveBeginPlay`
  (bind _returnvalue (`SceneComponent.K2_GetComponentLocation` (`self.RadialForce`)))
  (`KismetSystemLibrary.Delay` 0.55)
  (`GameplayStatics.SpawnEmitterAtLocation` "/Game/kosm_fps_assets/Misc/Particles/P_BubbleBurst2.P_BubbleBurst2" (`self.K2_GetActorLocation`) (struct) (4.0 4.0 4.0))
  (`GameplayStatics.ApplyRadialDamage` :`BaseDamage` 50.0 :`Origin` (`self.K2_GetActorLocation`) :`DamageRadius` 1200.0 :`DamageCauser` null :`InstigatedByController` null)
  (`RadialForceComponent.FireImpulse` (`self.RadialForce`))
  (`GameplayStatics.PlaySoundAtLocation` "/Game/AUDIO/SFX_Weapons/Weap_Bubblegun/SC_Energy_Explosion.SC_Energy_Explosion" _returnvalue (struct) 1.0 1.0 0.0 null null null)
  (`GameplayStatics.PlayWorldCameraShake` "/Game/Blueprints/SHAKES/BP_CameraShake_Jump_Heavy.BP_CameraShake_Jump_Heavy_C" _returnvalue 900.0 1000.0)
  (`self.K2_DestroyActor`))

(event `self.ReceiveHit`
  (params (MyComp :type "PrimitiveComponent Object Reference") (Other :type "Actor Object Reference") (OtherComp :type "PrimitiveComponent Object Reference") (bSelfMoved :type Boolean) (HitLocation :type "Vector Structure") (HitNormal :type "Vector Structure") (NormalImpulse :type "Vector Structure") (Hit :type "HitResult Structure (by ref)"))
  (bind _radialforce (`self.RadialForce`))
  (`KismetSystemLibrary.Delay` 8.0)
  (if (`|EnumInequality` (`SceneComponent.Mobility` OtherComp) "Movable")
    (`/Engine/EditorBlueprintResources/StandardMacros.IsValid` OtherComp
      (:`Is Valid`
        (bind _returnvalue (`GameplayStatics.SpawnDecalAttached` "/Game/kosm_fps_assets/Misc/Materials/BulletHole001.BulletHole001" (25.0 25.0 25.0) OtherComp "None" (`KismetMathLibrary.InverseTransformLocation` (`SceneComponent.K2_GetComponentToWorld` OtherComp) HitLocation) (`KismetMathLibrary.Conv_VectorToRotator` HitNormal) "KeepRelativeOffset" 30.0))
        (`DecalComponent.SetFadeScreenSize` _returnvalue 0.001))
      (:`Is Not Valid`
        _))
    (`GameplayStatics.SpawnEmitterAtLocation` "/Game/kosm_fps_assets/Misc/Particles/P_BubbleBurst2.P_BubbleBurst2" (`self.K2_GetActorLocation`) (struct) (4.0 4.0 4.0) :!label _label)
    (`GameplayStatics.ApplyRadialDamage` :`BaseDamage` 30.0 :`Origin` (`self.K2_GetActorLocation`) :`DamageRadius` 800.0 :`DamageCauser` self :`InstigatedByController` (`self.GetInstigatorController`))
    (`/Engine/EditorBlueprintResources/StandardMacros.IsValid` _radialforce
      (:`Is Valid`
        (`RadialForceComponent.FireImpulse` _radialforce)
        (`GameplayStatics.PlaySoundAtLocation` "/Game/AUDIO/SFX_Weapons/Weap_Bubblegun/SC_Energy_Explosion.SC_Energy_Explosion" (`SceneComponent.K2_GetComponentLocation` (`self.RadialForce`)) (struct) 1.0 1.0 0.0 null null null))
      (:`Is Not Valid`
        _))
    (`GameplayStatics.PlayWorldCameraShake` "/Game/Blueprints/SHAKES/BP_CameraShake_Jump_Heavy.BP_CameraShake_Jump_Heavy_C" (0.0 0.0 0.0) 900.0 1000.0)
    (`self.K2_DestroyActor`)))

(event `self.Sphere.OnComponentBeginOverlap`
  (params (OverlappedComponent :type "PrimitiveComponent Object Reference") (OtherActor :type "Actor Object Reference") (OtherComp :type "PrimitiveComponent Object Reference") (OtherBodyIndex :type Integer) (bFromSweep :type Boolean) (SweepResult :type "HitResult Structure (by ref)"))
  (if (!= OtherActor (`self.GetInstigator`))
    (goto _label)))

(event `self.ProjectileMovement.OnProjectileBounce`
  (params (ImpactResult :type "HitResult Structure (by ref)") (ImpactVelocity :type "Vector Structure (by ref)"))
  (bind _returnvalue (`self.K2_GetActorLocation`))
  (bind _returnvalue_2 (`SceneComponent.K2_GetComponentLocation` (`self.StaticMesh`)))
  (if (== (`self.BounceNumber`) 2.0)
    (`GameplayStatics.SpawnEmitterAtLocation` "/Game/kosm_fps_assets/Misc/Particles/P_BubbleBurst2.P_BubbleBurst2" _returnvalue (struct) (4.0 4.0 4.0))
    (`GameplayStatics.ApplyRadialDamage` :`BaseDamage` 30.0 :`Origin` _returnvalue :`DamageRadius` 800.0 :`DamageCauser` null :`InstigatedByController` null)
    (`RadialForceComponent.FireImpulse` (`self.RadialForce`))
    (`GameplayStatics.PlaySoundAtLocation` "/Game/AUDIO/SFX_Weapons/Weap_Bubblegun/SC_Energy_Explosion.SC_Energy_Explosion" _returnvalue_2 (struct) 1.0 1.0 0.0 null null null)
    (`GameplayStatics.PlayWorldCameraShake` "/Game/Blueprints/SHAKES/BP_CameraShake_Jump_Heavy.BP_CameraShake_Jump_Heavy_C" _returnvalue_2 900.0 1000.0)
    (`self.K2_DestroyActor`)
    (else
      (`GameplayStatics.PlaySoundAtLocation` "/Game/AUDIO/SFX_Weapons/Weap_Bubblegun/SC_Energy_Bounce.SC_Energy_Bounce" (`SceneComponent.K2_GetComponentLocation` (`self.RadialForce`)) (struct) 1.5 1.0 0.0 null null null)
      (set `self.BounceNumber` (+ (`self.BounceNumber`) 1.0)))))

(fn `UserConstructionScript`)