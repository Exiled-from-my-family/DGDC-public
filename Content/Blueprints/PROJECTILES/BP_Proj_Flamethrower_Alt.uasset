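; Short-lived alternate flamethrower projectile that deals fixed damage to ep1_character actors overlapping its box.
; On spawn it stores its location, prints the player's PlasmaCharge and enables box CCD after a brief delay.
; The authority copy destroys itself after a short delay, while remote copies destroy immediately.
; Overlaps apply damage only if a debug-drawn visibility trace back to the spawn point is clear, preventing damage through walls.
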(event `self.ReceiveBeginPlay`
  (`|ExecutionSequence`
    (:`then_0`
      (set `self.NewVar_0` (`self.K2_GetActorLocation`))
      (bind _player (`/Game/Blueprints/NewFunctionLibrary.get player`))
      (`KismetSystemLibrary.PrintString` (`KismetStringLibrary.Conv_IntToString` (`/Game/Blueprints/CHARACTERS/fpsMovementCharacter_light_1_vq3.PlasmaCharge` _player)) true false)
      (`/Engine/EditorBlueprintResources/ActorMacros.Switch Has Authority`
        (:`Authority`
          (`KismetSystemLibrary.Delay` 0.4)
          (`self.K2_DestroyActor`))
        (:`Remote`
          (`self.K2_DestroyActor`))))
    (:`then_1`
      (`KismetSystemLibrary.Delay` 0.02)
      (`PrimitiveComponent.SetUseCCD` (`self.Box`) true "None"))))

(event `self.Box.OnComponentBeginOverlap`
  (params (OverlappedComponent :type "PrimitiveComponent Object Reference") (OtherActor :type "Actor Object Reference") (OtherComp :type "PrimitiveComponent Object Reference") (OtherBodyIndex :type Integer) (bFromSweep :type Boolean) (SweepResult :type "HitResult Structure (by ref)"))
  (bind _asep_1_character (cast `/Game/MISSIONS/EP1/Characters/ep1_character` OtherActor))
  (bind _player (`/Game/Blueprints/NewFunctionLibrary.get player`))
  (bind (_outhit _returnvalue) (`KismetSystemLibrary.LineTraceSingle` (`self.K2_GetActorLocation` _asep_1_character) (`self.NewVar_0`) "TraceTypeQuery1" false (`|MakeArray` OtherActor _player :!type "Actor Object Reference") "ForDuration"))
  ;[1 1 1] Checks for LOS so you can't dmg thru walls
  (if (not _returnvalue)
    (`GameplayStatics.ApplyDamage` _asep_1_character 8.0)))

(fn `UserConstructionScript`)