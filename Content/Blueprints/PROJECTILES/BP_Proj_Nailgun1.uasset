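; Nailgun projectile that deals small random radial damage on its first hit, sparing its instigator, then destroys itself with impact particles and sound.
; On spawn it traces forward and disables physics simulation unless a portal is ahead, then enables CCD after a short delay.
; Movable hits passing an Undead tag check get blood effects, while non-movable hits get crater decals.
; The headshot branch deals the same damage as body hits.
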(event `self.ReceiveBeginPlay`
  (bind _collisioncomponent (`self.CollisionComponent`))
  (bind _returnvalue (`SceneComponent.K2_GetComponentLocation` _collisioncomponent))
  ;[0.3687 0.5739 1] Begin Play / Apply Damage / Event Hit / Line Trace
  (`|ExecutionSequence`
    (:`then_0`
      (bind _outactors (`GameplayStatics.GetAllActorsWithTag` "Character"))
      (bind _outactors_2 (`GameplayStatics.GetAllActorsWithTag` "Projectile"))
      (`KismetArrayLibrary.Array_Append` _outactors_2 _outactors)
      (bind _outhit (`KismetSystemLibrary.LineTraceSingle` _returnvalue (+ _returnvalue (* (`KismetMathLibrary.GetForwardVector` (`SceneComponent.K2_GetComponentRotation` _collisioncomponent)) 100000.0)) "TraceTypeQuery1" false _outactors_2))
      (if (not (`.bSuccess` (cast `/Game/kosm_fps_assets/Misc/Portal/PortalBP` (`.HitActor` (`GameplayStatics.BreakHitResult` _outhit)) :!pure true)))
        (`PrimitiveComponent.SetSimulatePhysics` (`self.CollisionComponent`) false)))
    (:`then_1`
      (`KismetSystemLibrary.Delay` 0.02)
      (`PrimitiveComponent.SetUseCCD` (`self.CollisionComponent`) true "None"))))

(event `self.ReceiveHit`
  (params (MyComp :type "PrimitiveComponent Object Reference") (Other :type "Actor Object Reference") (OtherComp :type "PrimitiveComponent Object Reference") (bSelfMoved :type Boolean) (HitLocation :type "Vector Structure") (HitNormal :type "Vector Structure") (NormalImpulse :type "Vector Structure") (Hit :type "HitResult Structure (by ref)"))
  (bind _returnvalue (`KismetMathLibrary.RandomFloatInRange` 2.0 5.0))
  (bind (_bblockinghit _binitialoverlap _time _distance _location _impactpoint _normal _impactnormal _physmat _hitactor _hitcomponent _hitbonename) (`GameplayStatics.BreakHitResult` Hit))
  (bind _returnvalue_2 (`KismetMathLibrary.Conv_VectorToRotator` _normal))
  (bind _array (`|MakeArray` (`self.GetInstigator`) :!type "Actor Object Reference"))
  ;[0.3687 0.5739 1] Begin Play / Apply Damage / Event Hit / Line Trace
  (`/Engine/EditorBlueprintResources/StandardMacros.DoOnce` false
    (:`Completed`
      (if (== _hitbonename "head")
        (`GameplayStatics.ApplyRadialDamage` _returnvalue HitLocation 250.0 null _array self (`self.GetInstigatorController`))
        (else
          (`GameplayStatics.ApplyRadialDamage` _returnvalue HitLocation 250.0 null _array self (`self.GetInstigatorController`))))
      (`GameplayStatics.SpawnEmitterAtLocation` "/Game/kosm_fps_assets/Misc/Particles/P_NailgunImpact.P_NailgunImpact" (`self.K2_GetActorLocation`) (struct) (0.25 0.5 2.5))
      (`GameplayStatics.PlaySoundAtLocation` "/Game/AUDIO/SFX_Weapons/Weap_Nailgun/SC_Nailgun_Ricochet.SC_Nailgun_Ricochet" (`SceneComponent.K2_GetComponentLocation` (`self.RadialForce`)) (struct) 0.75 1.0 0.0 null null null)
      (`/Engine/EditorBlueprintResources/StandardMacros.IsValid` null
        (:`Is Valid`
          _)
        (:`Is Not Valid`
          _))
      (if (`|EnumEquality` (`SceneComponent.Mobility` OtherComp) "Movable")
        (if (`self.ActorHasTag` "Undead")
          (bind (_outhit _returnvalue_3) (`KismetSystemLibrary.LineTraceSingle` HitLocation (+ HitLocation (* (`KismetMathLibrary.GetUpVector` (`KismetMathLibrary.FindLookAtRotation` (`self.K2_GetActorLocation`) HitLocation)) -300.0)) "TraceTypeQuery1"))
          (if _returnvalue_3
            (bind (_bblockinghit_2 _binitialoverlap_2 _time_2 _distance_2 _location_2 _impactpoint_2 _normal_2) (`GameplayStatics.BreakHitResult` _outhit))
            (bind _returnvalue_4 (`GameplayStatics.SpawnDecalAtLocation` (select `int` (`KismetMathLibrary.RandomIntegerInRange` 0 7) :`0` "/Game/kosm_fps_assets/Misc/Materials/D_BloodStain_Inst.D_BloodStain_Inst" :`1` "/Game/kosm_fps_assets/Misc/Materials/D_BloodStain_Inst1.D_BloodStain_Inst1" :`2` "/Game/kosm_fps_assets/Misc/Materials/D_BloodStain_Inst2.D_BloodStain_Inst2" :`3` "/Game/kosm_fps_assets/Misc/Materials/D_BloodStain_Inst3.D_BloodStain_Inst3" :`4` "/Game/kosm_fps_assets/Misc/Materials/D_BloodStain_Inst4.D_BloodStain_Inst4" :`5` "/Game/kosm_fps_assets/Misc/Materials/D_BloodStain_Inst5.D_BloodStain_Inst5" :`6` "/Game/kosm_fps_assets/Misc/Materials/D_BloodStain_Inst6.D_BloodStain_Inst6" :`7` "/Game/kosm_fps_assets/Misc/Materials/D_BloodStain_Inst7.D_BloodStain_Inst7" :!type "MaterialInterface Object Reference") (`KismetMathLibrary.MakeVector` (`KismetMathLibrary.RandomFloatInRange` 120.0 150.0) (`KismetMathLibrary.RandomFloatInRange` 120.0 150.0) (`KismetMathLibrary.RandomFloatInRange` 120.0 150.0)) _location_2 (`KismetMathLibrary.MakeRotFromX` _normal_2) 10.0))
            (`DecalComponent.SetFadeScreenSize` _returnvalue_4 0.001))
          (`GameplayStatics.SpawnEmitterAttached` "/Game/kosm_fps_assets/Misc/Particles/PS_Blood_BulletHit1.PS_Blood_BulletHit1" null "None" (0.0 0.0 0.0) _returnvalue_2 (0.75 0.75 0.75)))
        (else
          (bind _returnvalue_5 (`GameplayStatics.SpawnDecalAttached` "/Game/kosm_fps_assets/Misc/Materials/D_Crater.D_Crater" (2.0 2.0 2.0) OtherComp "None" (0.0 0.0 0.0) _returnvalue_2 "SnapToTargetIncludingScale" 5.0))
          (`DecalComponent.SetFadeScreenSize` _returnvalue_5 0.001)))
      (`self.K2_DestroyActor`))))

(fn `IgnoreActorWhenMoving`
  (`PrimitiveComponent.IgnoreActorWhenMoving` (`self.CollisionComponent`) (`self.GetInstigator`) true))

(fn `UserConstructionScript`
  (`self.IgnoreActorWhenMoving`))