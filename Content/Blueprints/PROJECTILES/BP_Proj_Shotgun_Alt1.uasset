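; Shotgun alt-fire projectile that acts as a knockback blast through a forward box trace on spawn, run only on authority while remote copies destroy themselves.
; A hit non-Ghost character is launched upward, then forward after a brief delay, then takes small-radius damage that ignores Red Team actors.
; Ghost-tagged hits skip the launch and go straight to damage, and the projectile destroys itself after damaging.
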(event `self.ReceiveBeginPlay`
  (bind _collisioncomponent (`self.CollisionComponent`))
  (bind _returnvalue (`SceneComponent.K2_GetComponentLocation` _collisioncomponent))
  (`/Engine/EditorBlueprintResources/ActorMacros.Switch Has Authority`
    (:`Authority`
      (bind _outactors (`GameplayStatics.GetAllActorsWithTag` "Molly"))
      (bind (_outhit _returnvalue_2) (`KismetSystemLibrary.BoxTraceSingle` _returnvalue (+ _returnvalue (* (`KismetMathLibrary.GetForwardVector` (`SceneComponent.K2_GetComponentRotation` _collisioncomponent)) 4000.0)) (200.0 200.0 90.0) (struct) "TraceTypeQuery1" false _outactors "ForDuration"))
      (bind (_bblockinghit _binitialoverlap _time _distance _location _impactpoint _normal _impactnormal _physmat _hitactor) (`GameplayStatics.BreakHitResult` _outhit))
      (set `self.Range` _distance)
      (if _returnvalue_2
        (if (not (`self.ActorHasTag` _hitactor "Ghost"))
          (`KismetSystemLibrary.PrintString` "BOOP" true true (struct :`R` 1.0 :`G` 0.768674 :`A` 1.0))
          (bind _ascharacter (cast `Character` _hitactor))
          (`Character.LaunchCharacter` _ascharacter (0.0 0.0 1250.0) false false)
          (`KismetSystemLibrary.Delay` 0.1)
          (`Character.LaunchCharacter` _ascharacter (* (`SceneComponent.GetForwardVector` (`self.CollisionComponent`)) 3600.0) true false)
          (bind _outactors_2 (`GameplayStatics.GetAllActorsWithTag` "Red Team"))
          (else
            (`KismetSystemLibrary.PrintString` "NO BOOP" true false)))
        (`GameplayStatics.ApplyRadialDamage` 20.0 _impactpoint 1.0 null _outactors_2 self (`self.GetInstigatorController`) true)
        (`self.K2_DestroyActor`)))
    (:`Remote`
      (`self.K2_DestroyActor`))))

(fn `IgnoreActorWhenMoving`
  (`PrimitiveComponent.IgnoreActorWhenMoving` (`self.CollisionComponent`) (`self.GetInstigator`) true))

(fn `UserConstructionScript`
  (`self.IgnoreActorWhenMoving`))