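; Nailgun projectile that launches at high speed with random spread and deals small radial damage on its first hit.
; On spawn it turns off physics simulation unless a forward trace finds a portal, enables CCD after a brief delay and grows its collision sphere.
; Damage skips the instigator, Red Team and, in team mode, the player.
; Movable undead targets get blood effects; non-movable surfaces get a crater and a fading light before destruction.
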(event `self.ReceiveBeginPlay`
  (bind _projectile (`self.Projectile`))
  (bind _spread (`self.Spread`))
  (bind _collisioncomponent (`self.CollisionComponent`))
  (bind _returnvalue (`SceneComponent.K2_GetComponentLocation` _collisioncomponent))
  (bind _returnvalue_2 (* _spread -1.0))
  ;[0.3687 0.5739 1] Begin Play / Apply Damage / Event Hit / Line Trace
  (set `ProjectileMovementComponent.bRotationFollowsVelocity` true _projectile)
  (`ProjectileMovementComponent.SetVelocityInLocalSpace` _projectile (`KismetMathLibrary.MakeVector` 75000.0 (`KismetMathLibrary.RandomFloatInRange` _returnvalue_2 _spread) (`KismetMathLibrary.RandomFloatInRange` _returnvalue_2 _spread))) ; old X value: 35000
  (`|ExecutionSequence`
    (:`then_0`
      (bind _outactors (`GameplayStatics.GetAllActorsWithTag` "Character"))
      (bind _outactors_2 (`GameplayStatics.GetAllActorsWithTag` "Projectile"))
      (`KismetArrayLibrary.Array_Append` _outactors_2 _outactors)
      (bind _outhit (`KismetSystemLibrary.LineTraceSingle` _returnvalue (+ _returnvalue (* (`KismetMathLibrary.GetForwardVector` (`SceneComponent.K2_GetComponentRotation` _collisioncomponent)) 100000.0)) "TraceTypeQuery1" false _outactors_2))
      (if (not (`.bSuccess` (cast `/Game/kosm_fps_assets/Misc/Portal/PortalBP` (`.HitActor` (`GameplayStatics.BreakHitResult` _outhit)) :!pure true)))
        (`PrimitiveComponent.SetSimulatePhysics` (`self.CollisionComponent`) false)))
    (:`then_1`
      (`KismetSystemLibrary.Delay` 0.02)
      (`PrimitiveComponent.SetUseCCD` (`self.CollisionComponent`) true "None"))
    (:`then_2`
      (bind (_direction _newtrack_0) (`Timeline|Timeline_0` :!via `PlayFromStart`)
        (:`Update`
          (`SphereComponent.SetSphereRadius` (`self.CollisionComponent`) (`KismetMathLibrary.Lerp` 0.0 28.0 _newtrack_0) true))))))

(event `self.ReceiveHit`
  (params (MyComp :type "PrimitiveComponent Object Reference") (Other :type "Actor Object Reference") (OtherComp :type "PrimitiveComponent Object Reference") (bSelfMoved :type Boolean) (HitLocation :type "Vector Structure") (HitNormal :type "Vector Structure") (NormalImpulse :type "Vector Structure") (Hit :type "HitResult Structure (by ref)"))
  (bind (_bblockinghit _binitialoverlap _time _distance _location _impactpoint _normal _impactnormal _physmat _hitactor) (`GameplayStatics.BreakHitResult` Hit))
  (bind _pointlight (`self.PointLight`))
  (bind _returnvalue (`KismetMathLibrary.InverseTransformLocation` (`SceneComponent.K2_GetComponentToWorld` OtherComp) HitLocation))
  (bind _returnvalue_2 (`SceneComponent.K2_GetComponentLocation` (`self.RadialForce`)))
  (bind _returnvalue_3 (`KismetMathLibrary.Conv_VectorToRotator` _normal))
  ;[0.3687 0.5739 1] Begin Play / Apply Damage / Event Hit / Line Trace
  (`/Engine/EditorBlueprintResources/StandardMacros.DoOnce` false
    (:`Completed`
      (bind _outactors (`GameplayStatics.GetAllActorsWithTag` "Red Team"))
      (`KismetArrayLibrary.Array_Append` _outactors (`|MakeArray` (`self.GetInstigator`) :!type "Actor Object Reference"))
      (bind _game_instance (`/Game/Blueprints/NewFunctionLibrary.dead game instance`))
      (if (`/Game/Blueprints/DeadGaemInstance.team mode?` _game_instance)
        (`KismetArrayLibrary.Array_Append` _outactors (`|MakeArray` (`GameplayStatics.GetPlayerPawn` 0) :!type "Actor Object Reference")))
      (`GameplayStatics.ApplyRadialDamage` 9.0 HitLocation 15.0 null _outactors self (`self.GetInstigatorController`) true)
      (`GameplayStatics.SpawnEmitterAtLocation` "/Game/kosm_fps_assets/Misc/Particles/P_NailgunImpact.P_NailgunImpact" (`self.K2_GetActorLocation`) (struct) (0.25 0.5 2.5))
      (`GameplayStatics.PlaySoundAtLocation` (select `EPhysicalSurface` "SurfaceType_Default" :`SurfaceType1` "/Game/AUDIO/SFX_Movement/SC_Footsteps_Concrete.SC_Footsteps_Concrete" :`SurfaceType2` "/Game/AUDIO/SFX_Movement/SC_Footsteps_Stone.SC_Footsteps_Stone" :`SurfaceType3` "/Game/AUDIO/SFX_Movement/SC_Footsteps_Metal1.SC_Footsteps_Metal1" :`SurfaceType4` "/Game/AUDIO/SFX_Movement/SC_Footsteps_Metal2.SC_Footsteps_Metal2" :`SurfaceType5` "/Game/AUDIO/SFX_Movement/SC_Footsteps_Carpet.SC_Footsteps_Carpet" :`SurfaceType6` "/Game/AUDIO/SFX_Movement/SC_Footsteps_Wood1.SC_Footsteps_Wood1" :`SurfaceType7` "/Game/AUDIO/SFX_Movement/SC_Footsteps_Wood2.SC_Footsteps_Wood2" :`SurfaceType8` "/Game/AUDIO/SFX_Movement/SC_Footsteps_Grass.SC_Footsteps_Grass" :`SurfaceType9` "/Game/AUDIO/SFX_Movement/SC_Footsteps_Water1.SC_Footsteps_Water1" :`SurfaceType10` "/Game/AUDIO/SFX_Movement/SC_Footsteps_Gravel.SC_Footsteps_Gravel" :`SurfaceType11` "/Game/AUDIO/SFX_Movement/SC_Footsteps_Sand.SC_Footsteps_Sand" :`SurfaceType12` "/Game/AUDIO/SFX_Movement/SC_Footsteps_Mud.SC_Footsteps_Mud" :!type "SoundBase Object Reference") _returnvalue_2 (struct) 1.0 1.0 0.0 null null null)
      (`GameplayStatics.PlaySoundAtLocation` "/Game/AUDIO/SFX_Weapons/Weap_Nailgun/SC_Nailgun_Ricochet.SC_Nailgun_Ricochet" _returnvalue_2 (struct) 0.75 1.0 0.0 null null null)
      (if (`|EnumEquality` (`SceneComponent.Mobility` OtherComp) "Movable")
        (if (`self.ActorHasTag` _hitactor "Undead")
          (bind (_outhit _returnvalue_4) (`KismetSystemLibrary.LineTraceSingle` HitLocation (+ HitLocation (* (`KismetMathLibrary.GetUpVector` (`KismetMathLibrary.FindLookAtRotation` (`self.K2_GetActorLocation`) HitLocation)) -300.0)) "TraceTypeQuery1"))
          (if _returnvalue_4
            (bind (_bblockinghit_2 _binitialoverlap_2 _time_2 _distance_2 _location_2 _impactpoint_2 _normal_2) (`GameplayStatics.BreakHitResult` _outhit))
            (bind _returnvalue_5 (`GameplayStatics.SpawnDecalAtLocation` (select `int` (`KismetMathLibrary.RandomIntegerInRange` 0 7) :`0` "/Game/kosm_fps_assets/Misc/Materials/D_BloodStain_Inst.D_BloodStain_Inst" :`1` "/Game/kosm_fps_assets/Misc/Materials/D_BloodStain_Inst1.D_BloodStain_Inst1" :`2` "/Game/kosm_fps_assets/Misc/Materials/D_BloodStain_Inst2.D_BloodStain_Inst2" :`3` "/Game/kosm_fps_assets/Misc/Materials/D_BloodStain_Inst3.D_BloodStain_Inst3" :`4` "/Game/kosm_fps_assets/Misc/Materials/D_BloodStain_Inst4.D_BloodStain_Inst4" :`5` "/Game/kosm_fps_assets/Misc/Materials/D_BloodStain_Inst5.D_BloodStain_Inst5" :`6` "/Game/kosm_fps_assets/Misc/Materials/D_BloodStain_Inst6.D_BloodStain_Inst6" :`7` "/Game/kosm_fps_assets/Misc/Materials/D_BloodStain_Inst7.D_BloodStain_Inst7" :!type "MaterialInterface Object Reference") (`KismetMathLibrary.MakeVector` (`KismetMathLibrary.RandomFloatInRange` 100.0 120.0) (`KismetMathLibrary.RandomFloatInRange` 100.0 120.0) (`KismetMathLibrary.RandomFloatInRange` 100.0 120.0)) _location_2 (`KismetMathLibrary.MakeRotFromX` _normal_2) 10.0))
            (`DecalComponent.SetFadeScreenSize` _returnvalue_5 0.001)
            (else
              (`GameplayStatics.SpawnEmitterAttached` "/Game/kosm_fps_assets/Misc/Particles/PS_Blood_BulletHit1.PS_Blood_BulletHit1" OtherComp "None" _returnvalue _returnvalue_3))))
        (`self.K2_DestroyActor` :!label _label)
        (else
          (bind _returnvalue_6 (`GameplayStatics.SpawnDecalAttached` "/Game/kosm_fps_assets/Misc/Materials/D_Crater.D_Crater" (2.0 2.0 2.0) OtherComp "None" _returnvalue _returnvalue_3 "SnapToTargetIncludingScale" 5.0))
          (`/Engine/EditorBlueprintResources/StandardMacros.IsValid` _returnvalue_6
            (:`Is Valid`
              (`DecalComponent.SetFadeScreenSize` _returnvalue_6 0.001))
            (:`Is Not Valid`
              _))
          (`|ExecutionSequence`
            (:`then_0`
              (`LightComponentBase.SetCastShadows` _pointlight false)
              (`SceneComponent.SetVisibility` (`self.ParticleSystem`) false false)
              (`SceneComponent.SetVisibility` (`self.nail`) false false)
              (`KismetSystemLibrary.Delay` 1.0)
              (goto _label))
            (:`then_1`
              (bind (_direction _lights_out) (`Timeline|Nail cooling off`)
                (:`Update`
                  (`LightComponent.SetIntensity` _pointlight (`KismetMathLibrary.Lerp` 100.0 0.0 _lights_out)))))))))))

(fn `IgnoreActorWhenMoving`
  (`PrimitiveComponent.IgnoreActorWhenMoving` (`self.CollisionComponent`) (`self.GetInstigator`) true))

(fn `UserConstructionScript`
  (`self.IgnoreActorWhenMoving`))