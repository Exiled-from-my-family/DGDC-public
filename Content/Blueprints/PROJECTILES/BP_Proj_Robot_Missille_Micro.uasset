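; Robot micro-missile projectile that explodes on impact or sphere overlap, with filters on the instigator and Robot tag.
; Sphere collision turns on shortly after spawn, and hits on non-movable components leave an attached, temporary crater decal.
; Explosions spawn particles, then apply radial damage, impulse and sound before hiding and destroying the actor after a delay.
; Hitting EP3_robot_big skips damage and destroys the missile immediately after the particle burst.
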(event `self.ReceiveBeginPlay`
  (bind _sphere (`self.Sphere`))
  (`PrimitiveComponent.SetCollisionEnabled` _sphere "NoCollision")
  (`KismetSystemLibrary.Delay` 0.05)
  (`PrimitiveComponent.SetCollisionEnabled` _sphere "QueryAndPhysics"))

(event `self.ReceiveHit`
  (params (MyComp :type "PrimitiveComponent Object Reference") (Other :type "Actor Object Reference") (OtherComp :type "PrimitiveComponent Object Reference") (bSelfMoved :type Boolean) (HitLocation :type "Vector Structure") (HitNormal :type "Vector Structure") (NormalImpulse :type "Vector Structure") (Hit :type "HitResult Structure (by ref)"))
  (bind _returnvalue (`self.GetInstigatorController`))
  (if (`|EnumInequality` (`SceneComponent.Mobility` OtherComp) "Movable")
    (`/Engine/EditorBlueprintResources/StandardMacros.IsValid` OtherComp
      (:`Is Valid`
        (`GameplayStatics.SpawnDecalAttached` "/Game/kosm_fps_assets/Misc/Materials/D_Crater.D_Crater" (50.0 50.0 50.0) OtherComp "None" (`KismetMathLibrary.InverseTransformLocation` (`SceneComponent.K2_GetComponentToWorld` OtherComp) HitLocation) (`KismetMathLibrary.Conv_VectorToRotator` HitNormal) "KeepRelativeOffset" 10.0)
        (`GameplayStatics.SpawnEmitterAtLocation` "/Game/kosm_fps_assets/Misc/Particles/P_Explode3.P_Explode3" (`self.K2_GetActorLocation`) (struct) (0.75 0.75 0.75) :!label _label)
        (if (not (`.bSuccess` (cast `/Game/MISSIONS/EP3/Characters/EP3_robot_big` Other :!pure true)))
          (`GameplayStatics.ApplyRadialDamage` 7.0 (`self.K2_GetActorLocation`) 300.0 null (`|MakeArray` _returnvalue :!type "Actor Object Reference") self _returnvalue)
          (`RadialForceComponent.FireImpulse` (`self.RadialForce`))
          (`ActorComponent.K2_DestroyComponent` (`self.RadialForce`))
          (`ActorComponent.K2_DestroyComponent` (`self.Audio`))
          (`ActorComponent.K2_DestroyComponent` (`self.ParticleSystem1`))
          (`SceneComponent.SetHiddenInGame` (`self.StaticMesh`) true false)
          (`self.SetActorEnableCollision` false)
          (`GameplayStatics.PlaySoundAtLocation` "/Game/AUDIO/SFX_Weapons/Weap_GrenadeLauncher/SC_Explosion_Flare.SC_Explosion_Flare" (`self.K2_GetActorLocation`) (struct) 0.5 1.5 0.0 null null null)
          (`KismetSystemLibrary.Delay` 1.0))
        (`self.K2_DestroyActor`))
      (:`Is Not Valid`
        (if (not (`self.ActorHasTag` Other "Robot"))
          (goto _label))))
    (else
      (goto _label))))

(event `self.Sphere.OnComponentBeginOverlap`
  (params (OverlappedComponent :type "PrimitiveComponent Object Reference") (OtherActor :type "Actor Object Reference") (OtherComp :type "PrimitiveComponent Object Reference") (OtherBodyIndex :type Integer) (bFromSweep :type Boolean) (SweepResult :type "HitResult Structure (by ref)"))
  (if (or (!= OtherActor (`self.GetInstigator`)) (not (`self.ActorHasTag` OtherActor "Robot")))
    (goto _label)))

(fn `UserConstructionScript`)