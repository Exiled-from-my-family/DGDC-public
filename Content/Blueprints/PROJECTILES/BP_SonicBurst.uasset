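; BP_SonicBurst is a short-lived visual effect actor that renders a heat-distortion burst on a sphere.
; The construction script gives the sphere a dynamic heat-distortion material with initial opacity and refraction.
; On BeginPlay, the Burst timeline drives scale, opacity and refraction from one track, with larger size paired with weaker distortion.
; The actor destroys itself when the timeline finishes.
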(event `self.ReceiveBeginPlay`
  (bind _sphere (`self.Sphere`))
  (bind (_direction _newtrack_0 _newtrack_1) (`Timeline|Burst` :!via `PlayFromStart`)
    (:`Update`
      (`SceneComponent.SetRelativeScale3D` _sphere (`KismetMathLibrary.VLerp` (20.0 20.0 20.0) (1.0 1.0 1.0) _newtrack_1))
      (`MeshComponent.SetScalarParameterValueOnMaterials` _sphere "Opacity" (`KismetMathLibrary.Lerp` 0.0 0.0075 _newtrack_1))
      (`MeshComponent.SetScalarParameterValueOnMaterials` _sphere "Refraction" (`KismetMathLibrary.Lerp` 0.0 6.0 _newtrack_1)))
    (:`Finished`
      (`self.K2_DestroyActor`))))

(fn `UserConstructionScript`
  (bind _sphere (`self.Sphere`))
  (`PrimitiveComponent.CreateDynamicMaterialInstance` _sphere 0 "/Game/kosm_fps_assets/Misc/Particles/Materials/M_Heat_Distortion.M_Heat_Distortion" "None")
  (`MeshComponent.SetScalarParameterValueOnMaterials` _sphere "Opacity" 0.05)
  (`MeshComponent.SetScalarParameterValueOnMaterials` _sphere "Refraction" 2.0))