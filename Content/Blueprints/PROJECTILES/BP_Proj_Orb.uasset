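; Bouncing energy orb projectile that zaps nearby living characters with beams and bursts in a radial explosion.
; A timeline drives mesh scale, light radius and damage radius together, then detonates the orb when finished.
; Tick sphere-traces that radius for throttled proximity damage, with an unused visibility trace.
; Overlapping a non-instigator or a delayed Hit also detonates it, with radial damage ignoring "Red Team" actors.
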(event `self.ReceiveBeginPlay`
  (bind _returnvalue (`SceneComponent.K2_GetComponentLocation` (`self.RadialForce`)))
  (`|ExecutionSequence`
    (:`then_0`
      (bind (_direction _bubble_squeeze) (`Timeline|Bubble start pop` :!via `PlayFromStart`)
        (:`Update`
          (set `self.DMG radius` (`KismetMathLibrary.Lerp` 1000.0 50.0 _bubble_squeeze))
          (`SceneComponent.SetRelativeScale3D` (`self.StaticMesh1`) (`KismetMathLibrary.VLerp` (1.5 1.5 1.5) (0.0 0.0 0.0) _bubble_squeeze))
          (`SceneComponent.SetRelativeScale3D` (`self.Sphere`) (`KismetMathLibrary.VLerp` (1.5 1.5 1.5) (0.0 0.0 0.0) _bubble_squeeze))
          (`LocalLightComponent.SetAttenuationRadius` (`self.PointLight`) (`KismetMathLibrary.Lerp` 1000.0 0.0 _bubble_squeeze)))
        (:`Finished`
          (`GameplayStatics.SpawnEmitterAtLocation` "/Game/kosm_fps_assets/Misc/Particles/P_BubbleBurst1.P_BubbleBurst1" (`self.K2_GetActorLocation`) (struct) (4.0 4.0 4.0))
          (`GameplayStatics.ApplyRadialDamage` 32.0 (`self.K2_GetActorLocation`) (`self.DMG radius`) null (stale `self.ReceiveBeginPlay` _outactors) null null)
          (`RadialForceComponent.FireImpulse` (`self.RadialForce`))
          (`GameplayStatics.PlaySoundAtLocation` "/Game/AUDIO/SFX_Weapons/Weap_Bubblegun/SC_Energy_Explosion.SC_Energy_Explosion" _returnvalue (struct) 1.0 1.0 0.0 null null null)
          (`GameplayStatics.PlayWorldCameraShake` "/Game/Blueprints/SHAKES/BP_CameraShake_Jump_Heavy.BP_CameraShake_Jump_Heavy_C" _returnvalue 900.0 1000.0)
          (`self.K2_DestroyActor`))))
    (:`then_1`
      (bind _outactors (`GameplayStatics.GetAllActorsWithTag` "Red Team")))))

(event `self.ReceiveHit`
  (params (MyComp :type "PrimitiveComponent Object Reference") (Other :type "Actor Object Reference") (OtherComp :type "PrimitiveComponent Object Reference") (bSelfMoved :type Boolean) (HitLocation :type "Vector Structure") (HitNormal :type "Vector Structure") (NormalImpulse :type "Vector Structure") (Hit :type "HitResult Structure (by ref)"))
  (bind _returnvalue (`SceneComponent.K2_GetComponentLocation` (`self.RadialForce`)))
  (`KismetSystemLibrary.Delay` 8.0)
  (if (`|EnumInequality` (`SceneComponent.Mobility` OtherComp) "Movable")
    (`/Engine/EditorBlueprintResources/StandardMacros.IsValid` OtherComp
      (:`Is Valid`
        (bind _returnvalue_2 (`GameplayStatics.SpawnDecalAttached` "/Game/kosm_fps_assets/Misc/Materials/BulletHole001.BulletHole001" (25.0 25.0 25.0) OtherComp "None" (`KismetMathLibrary.InverseTransformLocation` (`SceneComponent.K2_GetComponentToWorld` OtherComp) HitLocation) (`KismetMathLibrary.Conv_VectorToRotator` HitNormal) "KeepRelativeOffset" 30.0))
        (`DecalComponent.SetFadeScreenSize` _returnvalue_2 0.001))
      (:`Is Not Valid`
        _))
    (`GameplayStatics.SpawnEmitterAtLocation` "/Game/kosm_fps_assets/Misc/Particles/P_BubbleBurst1.P_BubbleBurst1" (`self.K2_GetActorLocation`) (struct) (4.0 4.0 4.0) :!label _label)
    (`GameplayStatics.ApplyRadialDamage` 32.0 (`self.K2_GetActorLocation`) (`self.DMG radius`) null (stale `self.ReceiveBeginPlay` _outactors) self (`self.GetInstigatorController`))
    (`RadialForceComponent.FireImpulse` (`self.RadialForce`))
    (`GameplayStatics.PlaySoundAtLocation` "/Game/AUDIO/SFX_Weapons/Weap_Bubblegun/SC_Energy_Explosion.SC_Energy_Explosion" _returnvalue (struct) 1.0 1.0 0.0 null null null)
    (`GameplayStatics.PlayWorldCameraShake` "/Game/Blueprints/SHAKES/BP_CameraShake_Jump_Heavy.BP_CameraShake_Jump_Heavy_C" _returnvalue 900.0 1000.0)
    (`self.K2_DestroyActor`)))

(event `self.Sphere.OnComponentBeginOverlap`
  (params (OverlappedComponent :type "PrimitiveComponent Object Reference") (OtherActor :type "Actor Object Reference") (OtherComp :type "PrimitiveComponent Object Reference") (OtherBodyIndex :type Integer) (bFromSweep :type Boolean) (SweepResult :type "HitResult Structure (by ref)"))
  (if (!= OtherActor (`self.GetInstigator`))
    (goto _label)))

(event `self.ProjectileMovement.OnProjectileBounce`
  (params (ImpactResult :type "HitResult Structure (by ref)") (ImpactVelocity :type "Vector Structure (by ref)"))
  (bind _returnvalue (`SceneComponent.K2_GetComponentLocation` (`self.RadialForce`)))
  (`GameplayStatics.PlaySoundAtLocation` "/Game/AUDIO/SFX_Weapons/Weap_Bubblegun/SC_Energy_Bounce.SC_Energy_Bounce" _returnvalue (struct) 1.5 1.0 0.0 null null null)
  (set `self.BounceNumber` (+ (`self.BounceNumber`) 1.0))
  (`GameplayStatics.SpawnEmitterAtLocation` "/Game/kosm_fps_assets/Misc/Particles/P_BubbleBurst1_1.P_BubbleBurst1_1" _returnvalue (struct :`Pitch` 90.0 :`Roll` 4905.0) (2.0 1.0 2.0)))

(event `self.ReceiveTick`
  (params (DeltaSeconds :type "Float (single-precision)"))
  (bind _returnvalue (`self.K2_GetActorLocation`))
  ;[0.81 0 1 1 32] WITHER AWAY (how prximity dmg is handled)
  (bind _player (`/Game/Blueprints/NewFunctionLibrary.get player`))
  (bind _outhits (`KismetSystemLibrary.SphereTraceMultiForObjects` _returnvalue _returnvalue (`self.DMG radius`) (`|MakeArray` "ObjectTypeQuery3" :!type "EObjectTypeQuery Enum") false (`|MakeArray` _player :!type "Actor Object Reference")))
  (for _array_element _outhits
    (bind (_asep_1_character _bsuccess) (cast `/Game/MISSIONS/EP1/Characters/ep1_character` (`.HitActor` (`GameplayStatics.BreakHitResult` _array_element)) :!pure true))
    (if (and (not (`/Game/Blueprints/CHARACTERS/NoobotAI/Blueprints/AI_NoobotChar.IsDead?` _asep_1_character)) _bsuccess)
      (`|ExecutionSequence`
        (:`then_0`
          (bind _returnvalue_2 (`self.K2_GetActorLocation` _asep_1_character))
          (`KismetSystemLibrary.LineTraceSingle` (`self.K2_GetActorLocation`) _returnvalue_2 "TraceTypeQuery1")
          (bind _returnvalue_3 (`GameplayStatics.SpawnEmitterAttached` "/Game/kosm_fps_assets/Misc/Particles/Laser/PS_Beam.PS_Beam" (`self.Sphere`)))
          (`ParticleSystemComponent.SetBeamTargetPoint` _returnvalue_3 0 _returnvalue_2 0))
        (:`then_1`
          (`/Engine/EditorBlueprintResources/StandardMacros.DoOnce` false :!label _label_2
            (:`Completed`
              (`GameplayStatics.ApplyDamage` _asep_1_character 3.0 (`GameplayStatics.GetPlayerController` 0) self)
              (`KismetSystemLibrary.Delay` 0.1)
              (goto _label_2 :!via `Reset`))))))))

(fn `UserConstructionScript`)