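; Rocket launcher projectile that explodes on its first hit, applying a radial impulse and radial damage, doubled for head-bone hits.
; The hit also spawns explosion effects, impact decals and, on characters, blood, then destroys the actor.
; On BeginPlay, a forward trace disables physics simulation unless it hits a PortalBP, and CCD is enabled after a brief delay.
; The construction script makes collision ignore the instigator when moving.
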(event `self.ReceiveBeginPlay`
  (bind _collisioncomponent (`self.CollisionComponent`))
  (bind _returnvalue (`SceneComponent.K2_GetComponentLocation` _collisioncomponent))
  ;[0.3687 0.5739 1] Begin Play / Apply Damage / Event Hit / Line Trace
  (`|ExecutionSequence`
    (:`then_0`
      (bind _outactors (`GameplayStatics.GetAllActorsWithTag` "Character"))
      (bind _outactors_2 (`GameplayStatics.GetAllActorsWithTag` "Projectile"))
      (`KismetArrayLibrary.Array_Append` _outactors_2 _outactors)
      (bind _outhit (`KismetSystemLibrary.LineTraceSingle` _returnvalue (+ _returnvalue (* (`KismetMathLibrary.GetForwardVector` (`SceneComponent.K2_GetComponentRotation` _collisioncomponent)) 100000.0)) "TraceTypeQuery1" false _outactors_2))
      (if (not (`.bSuccess` (cast `/Game/kosm_fps_assets/Misc/Portal/PortalBP` (`.HitActor` (`GameplayStatics.BreakHitResult` _outhit)) :!pure true)))
        (`PrimitiveComponent.SetSimulatePhysics` (`self.CollisionComponent`) false)))
    (:`then_1`
      (`KismetSystemLibrary.Delay` 0.02)
      (`PrimitiveComponent.SetUseCCD` (`self.CollisionComponent`) true "None"))))

(event `self.ReceiveHit`
  (params (MyComp :type "PrimitiveComponent Object Reference") (Other :type "Actor Object Reference") (OtherComp :type "PrimitiveComponent Object Reference") (bSelfMoved :type Boolean) (HitLocation :type "Vector Structure") (HitNormal :type "Vector Structure") (NormalImpulse :type "Vector Structure") (Hit :type "HitResult Structure (by ref)"))
  (bind (_bblockinghit _binitialoverlap _time _distance _location _impactpoint _normal _impactnormal _physmat _hitactor _hitcomponent _hitbonename) (`GameplayStatics.BreakHitResult` Hit))
  (bind _returnvalue (`KismetMathLibrary.Conv_VectorToRotator` _normal))
  (bind _returnvalue_2 (`KismetMathLibrary.MakeTransform` (0.0 0.0 0.0) _returnvalue))
  ;[0.3687 0.5739 1] Begin Play / Apply Damage / Event Hit / Line Trace
  (`/Engine/EditorBlueprintResources/StandardMacros.DoOnce` false
    (:`Completed`
      (`RadialForceComponent.FireImpulse` (`self.RadialForce`))
      (if (== _hitbonename "head")
        (`GameplayStatics.ApplyRadialDamage` :`BaseDamage` 92.0 :`Origin` HitLocation :`DamageRadius` 350.0 :`DamageCauser` self :`InstigatedByController` (`self.GetInstigatorController`))
        (else
          (`GameplayStatics.ApplyRadialDamage` :`BaseDamage` 46.0 :`Origin` HitLocation :`DamageRadius` 350.0 :`DamageCauser` self :`InstigatedByController` (`self.GetInstigatorController`))))
      (`GameplayStatics.SpawnEmitterAtLocation` "/Game/kosm_fps_assets/Misc/Particles/P_Explosion.P_Explosion" (`self.K2_GetActorLocation`) (struct) (5.0 5.0 5.0))
      (`GameplayStatics.PlaySoundAtLocation` "/Game/AUDIO/SFX_Weapons/Weap_GrenadeLauncher/SC_Explosion.SC_Explosion" (`SceneComponent.K2_GetComponentLocation` (`self.RadialForce`)) (struct) 0.75 1.0 0.0 null null null)
      (if (not (`self.ActorHasTag` _hitactor "Projectile"))
        (bind _returnvalue_3 (`GameplayStatics.SpawnDecalAttached` "/Game/kosm_fps_assets/Misc/Materials/BulletHole001.BulletHole001" (25.0 25.0 25.0) OtherComp "None" (`KismetMathLibrary.InverseTransformLocation` (`SceneComponent.K2_GetComponentToWorld` OtherComp) HitLocation) _returnvalue "KeepRelativeOffset" 30.0))
        (`DecalComponent.SetFadeScreenSize` _returnvalue_3 0.001)
        (if (`.bSuccess` (cast `Character` _hitactor :!pure true))
          (bind _returnvalue_4 (`GameplayStatics.SpawnDecalAtLocation` "/Game/kosm_fps_assets/Misc/Materials/D_BloodStain.D_BloodStain" (`KismetMathLibrary.MakeVector` (`KismetMathLibrary.RandomFloatInRange` 5.0 30.0) (`KismetMathLibrary.RandomFloatInRange` 5.0 30.0) (`KismetMathLibrary.RandomFloatInRange` 5.0 30.0)) _location (`KismetMathLibrary.MakeRotator` (`KismetMathLibrary.RandomFloatInRange` (.roll (.rotation _returnvalue_2)) 360.0) (.pitch (.rotation _returnvalue_2)) (.yaw (.rotation _returnvalue_2)))))
          (`SceneComponent.K2_AttachToComponent` _returnvalue_4 OtherComp _hitbonename "KeepWorld" "KeepWorld" "KeepWorld" true)
          (`DecalComponent.SetFadeScreenSize` _returnvalue_4 0.001)
          (`GameplayStatics.SpawnEmitterAttached` "/Game/kosm_fps_assets/Misc/Particles/PS_Blood_BulletHit.PS_Blood_BulletHit" OtherComp "None" (`KismetMathLibrary.InverseTransformLocation` (`SceneComponent.K2_GetComponentToWorld` OtherComp) HitLocation) _returnvalue (0.5 0.5 0.5))))
      (`self.K2_DestroyActor`))))

(fn `IgnoreActorWhenMoving`
  (`PrimitiveComponent.IgnoreActorWhenMoving` (`self.CollisionComponent`) (`self.GetInstigator`) true))

(fn `UserConstructionScript`
  (`self.IgnoreActorWhenMoving`))