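; Short-lived sand projectile effect that blinds any ep1_character overlapping its Cone, passing a value that shrinks as campaign difficulty rises.
; A timeline widens the visual Cone1 and drives its material opacity, then destroys it.
; In parallel, delays remove the overlap Cone and Decal early, limiting the blind window, then destroy the actor about a second after spawn.
; The construction script tints the decal and sets up the cone material.
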(event `self.ReceiveBeginPlay`
  (bind _returnvalue (`PrimitiveComponent.CreateDynamicMaterialInstance` (`self.Cone1`) 0 "/Game/Blueprints/PROJECTILES/M_LaserProj_Inst3.M_LaserProj_Inst3" "None"))
  (`|ExecutionSequence`
    (:`then_0`
      (bind (_direction _newtrack_0) (`Timeline|Timeline_0` :!via `PlayFromStart`)
        (:`Update`
          (`MaterialInstanceDynamic.SetScalarParameterValue` _returnvalue "Opacity" (`KismetMathLibrary.Lerp` -4.0 64.0 _newtrack_0))
          (`SceneComponent.SetRelativeScale3D` (`self.Cone1`) (`KismetMathLibrary.VLerp` (0.7 0.2 1.0) (1.8 1.1 1.0) _newtrack_0)))
        (:`Finished`
          (`ActorComponent.K2_DestroyComponent` (`self.Cone1`)))))
    (:`then_1`
      (`KismetSystemLibrary.Delay` 0.3)
      (`ActorComponent.K2_DestroyComponent` (`self.Cone`))
      (`ActorComponent.K2_DestroyComponent` (`self.Decal`))
      (`KismetSystemLibrary.Delay` 0.7)
      (`self.K2_DestroyActor`))))

(event `self.Cone.OnComponentBeginOverlap`
  (params (OverlappedComponent :type "PrimitiveComponent Object Reference") (OtherActor :type "Actor Object Reference") (OtherComp :type "PrimitiveComponent Object Reference") (OtherBodyIndex :type Integer) (bFromSweep :type Boolean) (SweepResult :type "HitResult Structure (by ref)"))
  (bind _asep_1_character (cast `/Game/MISSIONS/EP1/Characters/ep1_character` OtherActor))
  (bind _game_instance (`/Game/Blueprints/NewFunctionLibrary.dead game instance`))
  (`/Game/MISSIONS/EP1/Characters/ep1_character.BLINDED` _asep_1_character (select `/Game/DifficultyLevels_Campaign` (`/Game/Blueprints/DeadGaemInstance.difficulty campaign` _game_instance) :`NewEnumerator0` 3.5 :`NewEnumerator1` 2.5 :`NewEnumerator2` 1.5 :`NewEnumerator3` 1.0 :!type "Float (single-precision)")))

(fn `UserConstructionScript`
  (bind _returnvalue (`DecalComponent.CreateDynamicMaterialInstance` (`self.Decal`)))
  (`MaterialInstanceDynamic.SetVectorParameterValue` _returnvalue "Color" (struct :`R` 0.1 :`G` 0.080385 :`A` 1.0))
  (`MaterialInstanceDynamic.SetTextureParameterValue` _returnvalue "Mask" "/Game/MISSIONS/EP4/Blueprints/T_DropShadow_SQ3.T_DropShadow_SQ3")
  (`MaterialInstanceDynamic.SetScalarParameterValue` _returnvalue "mask strength" 0.0)
  (bind _returnvalue_2 (`PrimitiveComponent.CreateDynamicMaterialInstance` (`self.Cone1`) 0 "/Game/Blueprints/PROJECTILES/M_LaserProj_Inst3.M_LaserProj_Inst3" "None"))
  (`MaterialInstanceDynamic.SetScalarParameterValue` _returnvalue_2 "Opacity" 2.0))