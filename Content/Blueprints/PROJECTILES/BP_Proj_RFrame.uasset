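; RFrame bullet projectile that deals small-radius damage on impact, sparing Robot-tagged actors, then destroys itself.
; On spawn, a long forward trace turns off physics simulation unless it hits a PortalBP, and CCD is enabled after a brief delay.
; The first hit plays impact effects and sound, adding bullet holes on non-movable components, plus blood for Characters within that branch.
; The construction script makes collision ignore the instigator when moving.
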(event `self.ReceiveBeginPlay`
  (bind _collisioncomponent (`self.CollisionComponent`))
  (bind _returnvalue (`SceneComponent.K2_GetComponentLocation` _collisioncomponent))
  ;[0.3687 0.5739 1] Begin Play / Apply Damage / Event Hit / Line Trace
  (`|ExecutionSequence`
    (:`then_0`
      (bind _outactors (`GameplayStatics.GetAllActorsWithTag` "Character"))
      (bind _outactors_2 (`GameplayStatics.GetAllActorsWithTag` "Projectile"))
      (`KismetArrayLibrary.Array_Append` _outactors_2 _outactors)
      (bind _outhit (`KismetSystemLibrary.LineTraceSingle` _returnvalue (+ _returnvalue (* (`KismetMathLibrary.GetForwardVector` (`SceneComponent.K2_GetComponentRotation` _collisioncomponent)) 100000.0)) "TraceTypeQuery1" false _outactors_2))
      (if (not (`.bSuccess` (cast `/Game/kosm_fps_assets/Misc/Portal/PortalBP` (`.HitActor` (`GameplayStatics.BreakHitResult` _outhit)) :!pure true)))
        (`PrimitiveComponent.SetSimulatePhysics` (`self.CollisionComponent`) false)))
    (:`then_1`
      (`KismetSystemLibrary.Delay` 0.02)
      (`PrimitiveComponent.SetUseCCD` (`self.CollisionComponent`) true "None"))))

(event `self.ReceiveHit`
  (params (MyComp :type "PrimitiveComponent Object Reference") (Other :type "Actor Object Reference") (OtherComp :type "PrimitiveComponent Object Reference") (bSelfMoved :type Boolean) (HitLocation :type "Vector Structure") (HitNormal :type "Vector Structure") (NormalImpulse :type "Vector Structure") (Hit :type "HitResult Structure (by ref)"))
  (bind (_bblockinghit _binitialoverlap _time _distance _location _impactpoint _normal _impactnormal _physmat _hitactor) (`GameplayStatics.BreakHitResult` Hit))
  (bind _returnvalue (`KismetMathLibrary.InverseTransformLocation` (`SceneComponent.K2_GetComponentToWorld` OtherComp) HitLocation))
  (bind _returnvalue_2 (`KismetMathLibrary.Conv_VectorToRotator` _normal))
  (bind _returnvalue_3 (`KismetMathLibrary.MakeTransform` (0.0 0.0 0.0) _returnvalue_2))
  ;[0.3687 0.5739 1] Begin Play / Apply Damage / Event Hit / Line Trace
  (`/Engine/EditorBlueprintResources/StandardMacros.DoOnce` false
    (:`Completed`
      (bind _outactors (`GameplayStatics.GetAllActorsWithTag` "Robot"))
      (`GameplayStatics.ApplyRadialDamage` 7.0 HitLocation 25.0 null _outactors self (`self.GetInstigatorController`) true)
      (`GameplayStatics.SpawnEmitterAtLocation` "/Game/kosm_fps_assets/Misc/Particles/P_NailgunImpact.P_NailgunImpact" (`self.K2_GetActorLocation`) (struct) (0.25 0.5 2.5))
      (`GameplayStatics.PlaySoundAtLocation` "/Game/AUDIO/SFX_Weapons/Weap_Robots/SC_R-Frame_Ricochet.SC_R-Frame_Ricochet" (`SceneComponent.K2_GetComponentLocation` (`self.RadialForce`)) (struct) 0.5 1.0 0.0 null null null)
      (`/Engine/EditorBlueprintResources/StandardMacros.IsValid` null
        (:`Is Valid`
          (if (not (`|EnumEquality` (`SceneComponent.Mobility` OtherComp) "Movable"))
            (bind _returnvalue_4 (`GameplayStatics.SpawnDecalAttached` "/Game/kosm_fps_assets/Misc/Materials/BulletHole001.BulletHole001" (7.0 7.0 7.0) OtherComp "None" _returnvalue _returnvalue_2 "SnapToTargetIncludingScale" 30.0))
            (`DecalComponent.SetFadeScreenSize` _returnvalue_4 0.001)
            (if (`.bSuccess` (cast `Character` _hitactor :!pure true))
              (bind _returnvalue_5 (`GameplayStatics.SpawnDecalAtLocation` "/Game/kosm_fps_assets/Misc/Materials/D_BloodStain.D_BloodStain" (`KismetMathLibrary.MakeVector` (`KismetMathLibrary.RandomFloatInRange` 5.0 30.0) (`KismetMathLibrary.RandomFloatInRange` 5.0 30.0) (`KismetMathLibrary.RandomFloatInRange` 5.0 30.0)) _location (`KismetMathLibrary.MakeRotator` (`KismetMathLibrary.RandomFloatInRange` (.roll (.rotation _returnvalue_3)) 360.0) (.pitch (.rotation _returnvalue_3)) (.yaw (.rotation _returnvalue_3)))))
              (`DecalComponent.SetFadeScreenSize` _returnvalue_5 0.001)
              (`GameplayStatics.SpawnEmitterAttached` "/Game/kosm_fps_assets/Misc/Particles/PS_Blood_BulletHit.PS_Blood_BulletHit" OtherComp "None" _returnvalue _returnvalue_2 (0.5 0.5 0.5)))))
        (:`Is Not Valid`
          _))
      (`self.K2_DestroyActor`))))

(fn `IgnoreActorWhenMoving`
  (`PrimitiveComponent.IgnoreActorWhenMoving` (`self.CollisionComponent`) (`self.GetInstigator`) true))

(fn `UserConstructionScript`
  (`self.IgnoreActorWhenMoving`))