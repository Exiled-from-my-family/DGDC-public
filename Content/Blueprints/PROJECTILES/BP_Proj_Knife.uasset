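; Knife projectile that deals radial damage on its first hit, sparing its instigator.
; Hit stops physics on the collision and nail components, toggles both particle systems and plays a sound at the impact.
; It destroys itself on striking a living character, or after a crossbow impact sound on anything else; dead characters leave it in place.
; Unreachable leftover logic covers a banishment curse widget and an anti-necromancy kick.
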(event `self.ReceiveHit`
  (params (MyComp :type "PrimitiveComponent Object Reference") (Other :type "Actor Object Reference") (OtherComp :type "PrimitiveComponent Object Reference") (bSelfMoved :type Boolean) (HitLocation :type "Vector Structure") (HitNormal :type "Vector Structure") (NormalImpulse :type "Vector Structure") (Hit :type "HitResult Structure (by ref)"))
  (`/Engine/EditorBlueprintResources/StandardMacros.DoOnce` false
    (:`Completed`
      (`PrimitiveComponent.SetSimulatePhysics` (`self.CollisionComponent`) false)
      (`PrimitiveComponent.SetSimulatePhysics` (`self.nail`) false)
      (`SceneComponent.ToggleVisibility` (`self.ParticleSystem1`) false)
      (`SceneComponent.ToggleVisibility` (`self.ParticleSystem_0`) false)
      (`GameplayStatics.SpawnSoundAtLocation` null HitLocation (struct) 1.0 1.0 0.0 null null)
      (`/Game/Blueprints/NewFunctionLibrary.get player`)
      (`GameplayStatics.ApplyRadialDamage` (`self.damage`) HitLocation 250.0 null (`|MakeArray` (`self.GetInstigator`) :!type "Actor Object Reference") self (`self.GetInstigatorController`) true)
      (bind _asfps_movement_character_light_1_vq_3 (cast `/Game/Blueprints/CHARACTERS/fpsMovementCharacter_light_1_vq3` Other)
        (:`then`
          (if (not (`/Game/Blueprints/CHARACTERS/fpsMovementCharacter_light_1_vq3.IsDead?` _asfps_movement_character_light_1_vq_3))
            (`self.K2_DestroyActor` :!label _label)))
        (:`CastFailed`
          (`GameplayStatics.PlaySoundAtLocation` "/Game/AUDIO/SFX_Weapons/Weap_Crossbow/SC_Crossbow_Impact.SC_Crossbow_Impact" (`self.K2_GetActorLocation`) (struct) 0.25 1.0 0.0 null null null)
          (goto _label))))))

(fn `UserConstructionScript`
  (`parent.UserConstructionScript`))