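; Charged alt-fire SMG projectile that costs machinegun ammo and deals radial damage scaled by its DMGCharge.
; On spawn it draws a beam from the instigator's first-person muzzle along its forward vector, revealing a second beam only at full charge.
; Hits spawn a burst, then either overcharge a movable EP3_robot at full charge or leave impact effects and a decal on non-movable surfaces.
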(event `CustomEvent_0`
  (params (Start :type "Vector Structure") (End :type "Vector Structure"))
  (bind _returnvalue (`SceneComponent.K2_GetComponentLocation` (`/Game/Blueprints/CHARACTERS/fpsMovementCharacter_light_1_vq3.Muzzle1P` (cast `/Game/Blueprints/CHARACTERS/fpsMovementCharacter_light_1_vq3` (`self.GetInstigator`) :!pure true))))
  (`ParticleSystemComponent.SetBeamSourcePoint` (`self.ParticleSystem`) 0 _returnvalue 0)
  (`ParticleSystemComponent.SetBeamEndPoint` (`self.ParticleSystem`) 0 End)
  (`ParticleSystemComponent.SetBeamSourcePoint` (`self.ParticleSystem1`) 0 _returnvalue 0)
  (`ParticleSystemComponent.SetBeamEndPoint` (`self.ParticleSystem1`) 0 End))

(event `self.ReceiveBeginPlay`
  (bind _returnvalue (`SceneComponent.K2_GetComponentLocation` (`self.CollisionComponent`)))
  ;[0.3687 0.5739 1] Begin Play / Apply Damage / Event Hit / Line Trace
  (bind _player (`/Game/Blueprints/NewFunctionLibrary.get player`))
  (set `/Game/Blueprints/CHARACTERS/fpsMovementCharacter_light_1_vq3.MachinegunAmmo` (- (`/Game/Blueprints/CHARACTERS/fpsMovementCharacter_light_1_vq3.MachinegunAmmo` _player) 4) _player)
  (`KismetSystemLibrary.PrintString` (`KismetStringLibrary.Conv_DoubleToString` (`KismetMathLibrary.FClamp` (`KismetMathLibrary.SafeDivide` (`self.DMG charge`) 2.0) 5.0 100.0)) true false)
  (`self.CustomEvent_0` _returnvalue (+ (+ _returnvalue (* (`SceneComponent.GetForwardVector` (`self.CollisionComponent`)) 8000.0)) (0.0 0.0 0.0)))
  (`SceneComponent.SetHiddenInGame` (`self.ParticleSystem1`) (select `bool` (== (`self.DMG Charge`) 100.0) :`false` true) false))

(event `self.CollisionComponent.OnComponentHit`
  (params (HitComponent :type "PrimitiveComponent Object Reference") (OtherActor :type "Actor Object Reference") (OtherComp :type "PrimitiveComponent Object Reference") (NormalImpulse :type "Vector Structure") (Hit :type "HitResult Structure (by ref)"))
  (bind (_bblockinghit _binitialoverlap _time _distance _location _impactpoint _normal _impactnormal _physmat _hitactor _hitcomponent) (`GameplayStatics.BreakHitResult` Hit))
  (bind (_asep3_robot _bsuccess) (cast `/Game/MISSIONS/EP3/Characters/EP3_robot` _hitactor :!pure true))
  ;[0.3687 0.5739 1] Begin Play / Apply Damage / Event Hit / Line Trace
  (`GameplayStatics.ApplyRadialDamage` :`BaseDamage` (`KismetMathLibrary.FClamp` (`KismetMathLibrary.SafeDivide` (`self.DMG charge`) 2.0) 5.0 100.0) :`Origin` _location :`DamageRadius` 150.0 :`DamageCauser` self :`InstigatedByController` (`self.GetInstigatorController`) :`bDoFullDamage` true)
  (`|SpawnActorFromClass` "/Game/Blueprints/PROJECTILES/BP_HitBurst.BP_HitBurst_C" (`KismetMathLibrary.MakeTransform` _location (struct) (0.2 0.2 0.2)) "Undefined" "OverrideRootScale" null (1.0 0.1 0.0) null)
  (if (`|EnumEquality` (`SceneComponent.Mobility` _hitcomponent) "Movable")
    (if (and _bsuccess (== (`self.DMG Charge`) 100.0))
      (`/Game/MISSIONS/EP3/Characters/EP3_robot.Overcharge` _asep3_robot))
    (else
      (`GameplayStatics.SpawnEmitterAtLocation` "/Game/kosm_fps_assets/Misc/Particles/P_MinigunImpact.P_MinigunImpact" _location (struct) (0.75 0.75 0.75))
      (`GameplayStatics.PlaySoundAtLocation` "/Game/AUDIO/SFX_Weapons/Weap_Minigun/SC_Minigun_Ricochet.SC_Minigun_Ricochet" _location (struct) 1.0 1.0 0.0 null null null)
      (bind _returnvalue (`GameplayStatics.SpawnDecalAttached` "/Game/kosm_fps_assets/Misc/Materials/BulletHole001.BulletHole001" (4.0 4.0 4.0) _hitcomponent "None" (`KismetMathLibrary.InverseTransformLocation` (`SceneComponent.K2_GetComponentToWorld` _hitcomponent) _location) (`KismetMathLibrary.Conv_VectorToRotator` _normal) "KeepRelativeOffset" 30.0))
      (`DecalComponent.SetFadeScreenSize` _returnvalue 0.001)))
  (`KismetSystemLibrary.Delay` 2.0)
  (`self.K2_DestroyActor`))

(event `self.StaticMesh.OnComponentHit`
  (params (HitComponent :type "PrimitiveComponent Object Reference") (OtherActor :type "Actor Object Reference") (OtherComp :type "PrimitiveComponent Object Reference") (NormalImpulse :type "Vector Structure") (Hit :type "HitResult Structure (by ref)"))
  (`ActorComponent.K2_DestroyComponent` (`self.StaticMesh`)))

(fn `IgnoreActorWhenMoving`
  (`PrimitiveComponent.IgnoreActorWhenMoving` (`self.CollisionComponent`) (`self.GetInstigator`) true))

(fn `UserConstructionScript`
  (`self.IgnoreActorWhenMoving`))