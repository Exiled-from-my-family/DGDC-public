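; Sonic gun primary-fire projectile that acts as a hitscan shot, running two sphere traces on BeginPlay with authority and destroying remote copies.
; A short trace hit launches the player up, then backwards from the camera for a close-range boost.
; A long trace hit deals radial damage, reduced at range, spawns burst effects, then destroys the actor.
; Hit and overlap events are empty, leaving the target-knockback logic unreachable.
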(event `self.ReceiveBeginPlay`
  (bind _collisioncomponent (`self.CollisionComponent`))
  (bind _collisioncomponent_2 (`self.CollisionComponent`))
  (bind _returnvalue (`SceneComponent.K2_GetComponentLocation` _collisioncomponent))
  (bind _returnvalue_2 (`SceneComponent.K2_GetComponentLocation` _collisioncomponent_2))
  (bind _returnvalue_3 (`KismetMathLibrary.GetForwardVector` (`SceneComponent.K2_GetComponentRotation` _collisioncomponent_2)))
  (bind _returnvalue_4 (`KismetMathLibrary.GetForwardVector` (`SceneComponent.K2_GetComponentRotation` _collisioncomponent)))
  (`/Engine/EditorBlueprintResources/ActorMacros.Switch Has Authority`
    (:`Authority`
      (set `self.StartLocation` (`SceneComponent.K2_GetComponentLocation` (`self.CollisionComponent`)))
      (`|ExecutionSequence`
        (:`then_0`
          (bind (_outhit _returnvalue_5) (`KismetSystemLibrary.SphereTraceSingle` (+ _returnvalue_2 (* _returnvalue_3 20.0)) (+ _returnvalue_2 (* _returnvalue_3 500.0)) 10.0 "TraceTypeQuery1" false (`|MakeArray` (`GameplayStatics.GetPlayerCharacter` 0) :!type "Actor Object Reference")))
          (if _returnvalue_5
            (bind _player (`/Game/Blueprints/NewFunctionLibrary.get player`))
            (bind _charactermovement (`Character.CharacterMovement` _player))
            (set `CharacterMovementComponent.GroundFriction` 0.0 _charactermovement)
            (`Character.LaunchCharacter` _player (0.0 0.0 1100.0) false false)
            (`KismetSystemLibrary.Delay` 0.1)
            (`Character.LaunchCharacter` _player (* (`KismetMathLibrary.GetForwardVector` (`PlayerCameraManager.GetCameraRotation` (`GameplayStatics.GetPlayerCameraManager` 0))) -1850.0) false false)
            (set `CharacterMovementComponent.GroundFriction` 8.0 _charactermovement)))
        (:`then_1`
          (bind (_outhit_2 _returnvalue_6) (`KismetSystemLibrary.SphereTraceSingle` (+ _returnvalue (* _returnvalue_4 20.0)) (+ _returnvalue (* _returnvalue_4 1000000.0)) 35.0 "TraceTypeQuery1" false (`|MakeArray` (`GameplayStatics.GetPlayerCharacter` 0) :!type "Actor Object Reference") "ForDuration"))
          (if _returnvalue_6
            (`KismetSystemLibrary.PrintString` "NO BOOP" true false)
            (bind (_bblockinghit _binitialoverlap _time _distance _location _impactpoint _normal _impactnormal _physmat _hitactor _hitcomponent) (`GameplayStatics.BreakHitResult` _outhit_2))
            (`GameplayStatics.ApplyRadialDamage` (`KismetMathLibrary.SelectFloat` 25.0 45.0 (> (`KismetMathLibrary.Vector_Distance` (`self.StartLocation`) _impactpoint) 2500.0)) _impactpoint 50.0 null (`|MakeArray` (`/Game/Blueprints/NewFunctionLibrary.get player PURE`) :!type "Actor Object Reference") self (`self.GetInstigatorController`) true "ECC_GameTraceChannel2")
            (`GameplayStatics.SpawnEmitterAtLocation` "/Game/kosm_fps_assets/Misc/Particles/P_IceBurst1.P_IceBurst1" _impactpoint (struct) (2.0 2.0 2.0))
            (`/Game/MISSIONS/EP1/BP_MyMacroLibrary.For Loop With Delay` 0 2 0.05
              (:`Loop Body`
                (`|SpawnActorFromClass` "/Game/Blueprints/PROJECTILES/BP_SonicBurst.BP_SonicBurst_C" (`KismetMathLibrary.MakeTransform` (stale `self.ReceiveHit` HitLocation) (struct) (0.3 0.3 0.3)) "Undefined" "OverrideRootScale" null null))
              (:`Completed`
                (`KismetSystemLibrary.Delay` 1.0)
                (`self.K2_DestroyActor`)))))))
    (:`Remote`
      (`self.K2_DestroyActor`))))

(event `self.CollisionComponent.OnComponentBeginOverlap`
  (params (OverlappedComponent :type "PrimitiveComponent Object Reference") (OtherActor :type "Actor Object Reference") (OtherComp :type "PrimitiveComponent Object Reference") (OtherBodyIndex :type Integer) (bFromSweep :type Boolean) (SweepResult :type "HitResult Structure (by ref)")))

(event `self.ReceiveHit`
  (params (MyComp :type "PrimitiveComponent Object Reference") (Other :type "Actor Object Reference") (OtherComp :type "PrimitiveComponent Object Reference") (bSelfMoved :type Boolean) (HitLocation :type "Vector Structure") (HitNormal :type "Vector Structure") (NormalImpulse :type "Vector Structure") (Hit :type "HitResult Structure (by ref)")))

(fn `IgnoreActorWhenMoving`
  (`PrimitiveComponent.IgnoreActorWhenMoving` (`self.CollisionComponent`) (`self.GetInstigator`) true))

(fn `UserConstructionScript`
  (`self.IgnoreActorWhenMoving`))