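; Shotgun projectile that ignores its instigator when moving and deals radial damage on impact.
; Hit fires a one-time radial impulse and area damage, while mesh hits also fire the impulse, destroy the mesh and jump into the trace's close-headshot damage node.
; ShotgunLineTrace scales damage by distance and headshots, with impact, blood and bullet-hole effects.
; Its spread-randomised call is disconnected, leaving BeginPlay's six-pass authority loop empty.
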(event `ShotgunLineTrace`
  (params (TraceStart :type "Vector Structure") (TraceEnd :type "Vector Structure"))
  (bind _returnvalue (`self.GetInstigatorController`))
  (bind _returnvalue_2 (`self.GetInstigatorController`))
  (bind _shotgunrange (`self.ShotgunRange`))
  (bind _shotgunrange_2 (`self.ShotgunRange`))
  ;[0.3687 0.5739 1] Begin Play / Apply Damage / Event Hit / Line Trace
  (bind (_outhit _returnvalue_3) (`KismetSystemLibrary.LineTraceSingle` TraceStart TraceEnd "TraceTypeQuery1" false (`|MakeArray` (`self.OwningPawn`) (`self.Instigator`) :!type "Actor Object Reference") "Persistent" true (struct :`R` 1.0 :`A` 1.0) (struct :`G` 1.0 :`A` 1.0) 2.0))
  (bind (_bblockinghit _binitialoverlap _time _distance _location _impactpoint _normal _impactnormal _physmat _hitactor _hitcomponent _hitbonename _hititem _faceindex _tracestart) (`GameplayStatics.BreakHitResult` (stale `self.StaticMesh.OnComponentHit` Hit)))
  (set `self.ShotgunRange` _distance)
  (if (== _hitbonename "head")
    (if (<= _shotgunrange 500.0)
      (`GameplayStatics.ApplyRadialDamage` :`BaseDamage` 80.0 :`Origin` _location :`DamageRadius` 10.0 :`DamageCauser` self :`InstigatedByController` _returnvalue_2 :`bDoFullDamage` true :!label _label)
      (elif (<= _shotgunrange 2000.0)
        (`GameplayStatics.ApplyRadialDamage` :`BaseDamage` 32.0 :`Origin` _location :`DamageRadius` 10.0 :`DamageCauser` self :`InstigatedByController` _returnvalue_2 :`bDoFullDamage` true)
        (elif (<= _shotgunrange 8000.0)
          (`GameplayStatics.ApplyRadialDamage` :`BaseDamage` 20.0 :`Origin` _location :`DamageRadius` 10.0 :`DamageCauser` self :`InstigatedByController` _returnvalue_2 :`bDoFullDamage` true)
          (else
            (`GameplayStatics.ApplyRadialDamage` :`BaseDamage` 4.0 :`Origin` _location :`DamageRadius` 10.0 :`DamageCauser` self :`InstigatedByController` _returnvalue_2 :`bDoFullDamage` true)))))
    (elif (<= _shotgunrange_2 500.0)
      (`GameplayStatics.ApplyRadialDamage` :`BaseDamage` 40.0 :`Origin` _location :`DamageRadius` 10.0 :`DamageCauser` self :`InstigatedByController` _returnvalue :`bDoFullDamage` true)
      (elif (<= _shotgunrange_2 2000.0)
        (`GameplayStatics.ApplyRadialDamage` :`BaseDamage` 16.0 :`Origin` _location :`DamageRadius` 10.0 :`DamageCauser` self :`InstigatedByController` _returnvalue :`bDoFullDamage` true)
        (elif (<= _shotgunrange_2 8000.0)
          (`GameplayStatics.ApplyRadialDamage` :`BaseDamage` 10.0 :`Origin` _location :`DamageRadius` 10.0 :`DamageCauser` self :`InstigatedByController` _returnvalue :`bDoFullDamage` true)
          (else
            (`GameplayStatics.ApplyRadialDamage` :`BaseDamage` 2.0 :`Origin` _location :`DamageRadius` 10.0 :`DamageCauser` self :`InstigatedByController` _returnvalue :`bDoFullDamage` true))))))
  (`/Engine/EditorBlueprintResources/StandardMacros.IsValid` _hitactor
    (:`Is Valid`
      (`GameplayStatics.SpawnEmitterAtLocation` "/Game/kosm_fps_assets/Misc/Particles/P_Shotgun.P_Shotgun" _location :!label _label_2)
      (if (`.bSuccess` (cast `Character` _hitactor :!pure true))
        (bind _returnvalue_4 (`KismetMathLibrary.Conv_VectorToRotator` _normal))
        (`GameplayStatics.SpawnEmitterAttached` "/Game/kosm_fps_assets/Misc/Particles/PS_Blood_BulletHit.PS_Blood_BulletHit" _hitcomponent "None" (`KismetMathLibrary.InverseTransformLocation` (`SceneComponent.K2_GetComponentToWorld` _hitcomponent) _location) _returnvalue_4 (0.5 0.5 0.5))))
    (:`Is Not Valid`
      (if (`|EnumInequality` (`SceneComponent.Mobility` _hitcomponent) "Movable")
        (bind _returnvalue_5 (`GameplayStatics.SpawnDecalAttached` "/Game/kosm_fps_assets/Misc/Materials/BulletHole001.BulletHole001" (7.0 7.0 7.0) _hitcomponent "None" _location _returnvalue_4 "KeepRelativeOffset" 30.0))
        (else
          (goto _label_2))))))

(event `self.ReceiveBeginPlay`
  ;[0.3687 0.5739 1] Begin Play / Apply Damage / Event Hit / Line Trace
  (for _ (range 6)
    (`/Engine/EditorBlueprintResources/ActorMacros.Switch Has Authority`)))

(event `self.ReceiveHit`
  (params (MyComp :type "PrimitiveComponent Object Reference") (Other :type "Actor Object Reference") (OtherComp :type "PrimitiveComponent Object Reference") (bSelfMoved :type Boolean) (HitLocation :type "Vector Structure") (HitNormal :type "Vector Structure") (NormalImpulse :type "Vector Structure") (Hit :type "HitResult Structure (by ref)"))
  ;[0.3687 0.5739 1] Begin Play / Apply Damage / Event Hit / Line Trace
  (`/Engine/EditorBlueprintResources/StandardMacros.DoOnce` false
    (:`Completed`
      (`RadialForceComponent.FireImpulse` (`self.RadialForce`))
      (`GameplayStatics.ApplyRadialDamage` 32.0 HitLocation 250.0 null (`|MakeArray` (`self.GetInstigator`) :!type "Actor Object Reference") self (`self.GetInstigatorController`)))))

(event `self.StaticMesh.OnComponentHit`
  (params (HitComponent :type "PrimitiveComponent Object Reference") (OtherActor :type "Actor Object Reference") (OtherComp :type "PrimitiveComponent Object Reference") (NormalImpulse :type "Vector Structure") (Hit :type "HitResult Structure (by ref)"))
  ;[0.3687 0.5739 1] Begin Play / Apply Damage / Event Hit / Line Trace
  (`RadialForceComponent.FireImpulse` (`self.RadialForce`))
  (`ActorComponent.K2_DestroyComponent` (`self.StaticMesh`))
  (goto _label))

(fn `IgnoreActorWhenMoving`
  (`PrimitiveComponent.IgnoreActorWhenMoving` (`self.CollisionComponent`) (`self.GetInstigator`) true))

(fn `UserConstructionScript`
  (`self.IgnoreActorWhenMoving`))