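; Laser sight projectile for AI_NoobotChar that draws a beam from the weapon muzzle to where the projectile hits.
; BeginPlay sets the beam source once from the instigator's muzzle and destroys the actor on remote (non-authority) instances.
; The first Hit sets the beam target at the actor's location, then destroys it after a short delay.
; The construction script makes its collision ignore the instigator while moving.
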(event `self.ReceiveBeginPlay`
  ;[0.3687 0.5739 1] Begin Play / Apply Damage / Event Hit / Line Trace
  (bind _asai_noobot_char (cast `/Game/Blueprints/CHARACTERS/NoobotAI/Blueprints/AI_NoobotChar` (`self.GetInstigator`)))
  (`ParticleSystemComponent.SetBeamSourcePoint` (`self.ParticleSystem`) 0 (`SceneComponent.K2_GetComponentLocation` (`/Game/Blueprints/CHARACTERS/NoobotAI/Blueprints/AI_NoobotChar.WeaponMuzzle` _asai_noobot_char)) 0)
  (`/Engine/EditorBlueprintResources/ActorMacros.Switch Has Authority`
    (:`Remote`
      (`self.K2_DestroyActor`))))

(event `self.ReceiveHit`
  (params (MyComp :type "PrimitiveComponent Object Reference") (Other :type "Actor Object Reference") (OtherComp :type "PrimitiveComponent Object Reference") (bSelfMoved :type Boolean) (HitLocation :type "Vector Structure") (HitNormal :type "Vector Structure") (NormalImpulse :type "Vector Structure") (Hit :type "HitResult Structure (by ref)"))
  ;[0.3687 0.5739 1] Begin Play / Apply Damage / Event Hit / Line Trace
  (`/Engine/EditorBlueprintResources/StandardMacros.DoOnce` false
    (:`Completed`
      (`ParticleSystemComponent.SetBeamTargetPoint` (`self.ParticleSystem`) 0 (`self.K2_GetActorLocation`) 0)
      (`KismetSystemLibrary.Delay` 0.5)
      (`self.K2_DestroyActor`))))

(fn `IgnoreActorWhenMoving`
  (`PrimitiveComponent.IgnoreActorWhenMoving` (`self.CollisionComponent`) (`self.GetInstigator`) true))

(fn `UserConstructionScript`
  (`self.IgnoreActorWhenMoving`))