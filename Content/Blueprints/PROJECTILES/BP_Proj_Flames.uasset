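; BP_Proj_Flames is a ground fire hazard that snaps to the surface below on spawn, or destroys itself if none is found.
; After its duration, a timeline fades scale, light and audio, then destroys it.
; Sphere overlap calls OnFire on ep1_character and runs a limited, delayed damage loop on fpsMovementCharacter until it exits.
; Line traces let static geometry block both effects, with a leftover debug print for blocked ep1_characters.
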(event `self.ReceiveBeginPlay`
  (bind _returnvalue (`self.K2_GetActorLocation`))
  (bind (_outhit _returnvalue_2) (`KismetSystemLibrary.LineTraceSingle` _returnvalue (- _returnvalue (0.0 0.0 400.0)) "TraceTypeQuery1"))
  (if _returnvalue_2
    (`self.K2_SetActorLocation` (`.Location` (`GameplayStatics.BreakHitResult` _outhit)))
    (`KismetSystemLibrary.Delay` (`self.Duration`))
    (bind (_direction _newtrack_0) (`Timeline|Timeline_0` :!via `PlayFromStart`)
      (:`Update`
        (`SceneComponent.SetRelativeScale3D` (`self.DefaultSceneRoot`) (`KismetMathLibrary.VLerp` (1.0 1.0 1.0) (0.0 0.0 0.0) _newtrack_0))
        (`LightComponent.SetIntensity` (`self.PointLight`) (`KismetMathLibrary.Lerp` 32.0 0.0 _newtrack_0))
        (`AudioComponent.SetVolumeMultiplier` (`self.Audio`) (`KismetMathLibrary.Lerp` 1.0 0.0 _newtrack_0)))
      (:`Finished`
        (`self.K2_DestroyActor`)))
    (else
      (`self.K2_DestroyActor`))))

(event `self.Sphere.OnComponentBeginOverlap`
  (params (OverlappedComponent :type "PrimitiveComponent Object Reference") (OtherActor :type "Actor Object Reference") (OtherComp :type "PrimitiveComponent Object Reference") (OtherBodyIndex :type Integer) (bFromSweep :type Boolean) (SweepResult :type "HitResult Structure (by ref)"))
  (bind _asep_1_character (cast `/Game/MISSIONS/EP1/Characters/ep1_character` OtherActor)
    (:`then`
      (bind (_outhit _returnvalue) (`KismetSystemLibrary.LineTraceSingle` (+ (`self.K2_GetActorLocation`) (0.0 0.0 25.0)) (`self.K2_GetActorLocation` _asep_1_character) "TraceTypeQuery1"))
      (bind (_bblockinghit _binitialoverlap _time _distance _location _impactpoint _normal _impactnormal _physmat _hitactor _hitcomponent) (`GameplayStatics.BreakHitResult` _outhit))
      (`/Engine/EditorBlueprintResources/StandardMacros.IsValid` _hitcomponent
        (:`Is Valid`
          (if (and _returnvalue (`|EnumEquality` (`SceneComponent.Mobility` _hitcomponent) "Static"))
            (`KismetSystemLibrary.PrintString` "Hello")
            (else
              (`/Game/MISSIONS/EP1/Characters/ep1_character.OnFire` _asep_1_character null))))))
    (:`CastFailed`
      (bind _asfps_movement_character_light_1_vq_3 (cast `/Game/Blueprints/CHARACTERS/fpsMovementCharacter_light_1_vq3` OtherActor))
      (bind _output_get (set `self.player` _asfps_movement_character_light_1_vq_3))
      (`/Engine/EditorBlueprintResources/StandardMacros.DoOnce` false :!label _label
        (:`Completed`
          (`/Game/MISSIONS/EP1/BP_MyMacroLibrary.For Loop With Delay With Break` 0 9 0.5 :!label _label_2
            (:`Loop Body`
              (bind (_outhit_2 _returnvalue_2) (`KismetSystemLibrary.LineTraceSingle` (+ (`self.K2_GetActorLocation`) (0.0 0.0 25.0)) (`self.K2_GetActorLocation` _output_get) "TraceTypeQuery1"))
              (bind (_bblockinghit_2 _binitialoverlap_2 _time_2 _distance_2 _location_2 _impactpoint_2 _normal_2 _impactnormal_2 _physmat_2 _hitactor_2 _hitcomponent_2) (`GameplayStatics.BreakHitResult` _outhit_2))
              (`/Engine/EditorBlueprintResources/StandardMacros.IsValid` _hitcomponent_2
                (:`Is Valid`
                  (if (not (and _returnvalue_2 (`|EnumEquality` (`SceneComponent.Mobility` _hitcomponent_2) "Static")))
                    (`/Engine/EditorBlueprintResources/StandardMacros.IsValid` _output_get :!label _label_3
                      (:`Is Valid`
                        (`GameplayStatics.ApplyDamage` _output_get 5.0 (`self.GetInstigatorController`) self)))))
                (:`Is Not Valid`
                  (goto _label_3))))))))))

(event `self.Sphere.OnComponentEndOverlap`
  (params (OverlappedComponent :type "PrimitiveComponent Object Reference") (OtherActor :type "Actor Object Reference") (OtherComp :type "PrimitiveComponent Object Reference") (OtherBodyIndex :type Integer))
  (cast `/Game/Blueprints/CHARACTERS/fpsMovementCharacter_light_1_vq3` OtherActor)
  (`|ExecutionSequence`
    (:`then_0`
      (goto _label :!via `Reset`))
    (:`then_1`
      (goto _label_2 :!via `Break`))))

(fn `UserConstructionScript`)