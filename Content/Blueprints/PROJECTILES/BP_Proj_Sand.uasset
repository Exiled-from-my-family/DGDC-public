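; BP_Proj_Sand is a short-lived sand projectile actor whose graph drives a shrinking particle effect, with no movement or hit logic.
; On BeginPlay it randomly offsets its particle system, then the BubbleStartPop timeline interpolates its scale from large to zero via the BubbleSqueeze track.
; The actor destroys itself when the timeline finishes.
; A disconnected node chain for rotating toward the player pawn never runs.
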(event `self.ReceiveTick`
  (params (DeltaSeconds :type "Float (single-precision)")))

(event `self.ReceiveBeginPlay`
  (bind _returnvalue (`KismetMathLibrary.RandomFloatInRange` 2.0 10.0))
  (`SceneComponent.K2_SetRelativeLocation` (`self.ParticleSystem1`) (`KismetMathLibrary.MakeVector` _returnvalue _returnvalue _returnvalue) false false)
  (bind (_direction _bubble_squeeze) (`Timeline|Bubble start pop` :!via `PlayFromStart`)
    (:`Update`
      (`SceneComponent.SetRelativeScale3D` (`self.ParticleSystem1`) (`KismetMathLibrary.VLerp` (8.0 8.0 8.0) (0.0 0.0 0.0) _bubble_squeeze))
      (`KismetSystemLibrary.Delay` 0.55))
    (:`Finished`
      (`self.K2_DestroyActor`))))

(fn `UserConstructionScript`)