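; BP_IceVFX is a short-lived ice effect actor that shows an expanding, fading decal.
; On BeginPlay it creates a dynamic material for the decal, then a timeline drives its Opacity down and its scale up through two separate curves.
; The actor destroys itself when the timeline finishes.
; The sphere overlap event is empty, as the logic that slows ep1_character is left disconnected.
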(event `self.ReceiveBeginPlay`
  (bind _returnvalue (`DecalComponent.CreateDynamicMaterialInstance` (`self.Decal`)))
  (bind (_direction _ice _ice2) (`Timeline|Timeline_0` :!via `PlayFromStart`)
    (:`Update`
      (`MaterialInstanceDynamic.SetScalarParameterValue` _returnvalue "Strength" 0.5)
      (`MaterialInstanceDynamic.SetScalarParameterValue` _returnvalue "Opacity" (`KismetMathLibrary.Lerp` 3.0 0.0 _ice))
      (`SceneComponent.SetRelativeScale3D` (`self.Decal`) (`KismetMathLibrary.VLerp` (4.0 0.5 0.5) (6.0 5.0 5.0) _ice2)))
    (:`Finished`
      (`self.K2_DestroyActor`))))

(event `self.Sphere.OnComponentBeginOverlap`
  (params (OverlappedComponent :type "PrimitiveComponent Object Reference") (OtherActor :type "Actor Object Reference") (OtherComp :type "PrimitiveComponent Object Reference") (OtherBodyIndex :type Integer) (bFromSweep :type Boolean) (SweepResult :type "HitResult Structure (by ref)")))

(fn `UserConstructionScript`)