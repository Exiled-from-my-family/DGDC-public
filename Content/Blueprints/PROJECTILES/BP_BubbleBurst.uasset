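; BP_BubbleBurst is a short-lived effect actor that shows an expanding, fading bubble burst and then destroys itself.
; The construction script gives the Sphere a dynamic M_vegasLight material with full opacity.
; On BeginPlay the Burst timeline scales the sphere up about tenfold while lerping its opacity from faint to invisible, then destroys the actor when finished.
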(event `self.ReceiveBeginPlay`
  (bind _sphere (`self.Sphere`))
  (bind (_direction _newtrack_0) (`Timeline|Burst` :!via `PlayFromStart`)
    (:`Update`
      (`MeshComponent.SetScalarParameterValueOnMaterials` _sphere "opacity" (`KismetMathLibrary.Lerp` 0.25 0.0 _newtrack_0))
      (`SceneComponent.SetRelativeScale3D` _sphere (`KismetMathLibrary.VLerp` (2.0 2.0 2.0) (20.0 20.0 20.0) _newtrack_0)))
    (:`Finished`
      (`self.K2_DestroyActor`))))

(fn `UserConstructionScript`
  (bind _sphere (`self.Sphere`))
  (`PrimitiveComponent.CreateDynamicMaterialInstance` _sphere 0 "/Game/MATERIALS/M_vegasLight.M_vegasLight" "None")
  (`MeshComponent.SetScalarParameterValueOnMaterials` _sphere "opacity" 1.0))