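; Flashbang grenade projectile that plays a sound on each bounce and detonates one second after a hit.
; It searches actors of the movement character class and, for any living one within range, fades player 0's camera from white with audio fade.
; Detonation also removes its mesh and force components, disables collision, and plays explosion sound and particles.
; A fog cloud lingers for several seconds before the cloud and actor are destroyed.
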(event `self.ReceiveHit`
  (params (MyComp :type "PrimitiveComponent Object Reference") (Other :type "Actor Object Reference") (OtherComp :type "PrimitiveComponent Object Reference") (bSelfMoved :type Boolean) (HitLocation :type "Vector Structure") (HitNormal :type "Vector Structure") (NormalImpulse :type "Vector Structure") (Hit :type "HitResult Structure (by ref)"))
  (bind _returnvalue (`self.K2_GetActorLocation`))
  (`KismetSystemLibrary.Delay` 1.0)
  (`|ExecutionSequence`
    (:`then_0`
      (bind _outactors (`GameplayStatics.GetAllActorsOfClass` "/Game/Blueprints/CHARACTERS/fpsMovementCharacter_light_1_vq3.fpsMovementCharacter_light_1_vq3_C"))
      (for _array_element _outactors
        (if (and (not (`/Game/Blueprints/CHARACTERS/fpsMovementCharacter_light_1_vq3.IsDead?` _array_element)) (<= (`KismetMathLibrary.Vector_Distance` (`self.K2_GetActorLocation`) (`self.K2_GetActorLocation` _array_element)) 1250.0))
          (`KismetSystemLibrary.PrintString` "Hello")
          (`PlayerCameraManager.StartCameraFade` (`GameplayStatics.GetPlayerCameraManager` 0) 0.75 0.0 2.0 (struct :`R` 1.0 :`G` 1.0 :`B` 1.0 :`A` 1.0) true false))))
    (:`then_1`
      (`ActorComponent.K2_DestroyComponent` (`self.RadialForce`))
      (`ActorComponent.K2_DestroyComponent` (`self.StaticMesh`))
      (`self.SetActorEnableCollision` false)
      (`GameplayStatics.PlaySoundAtLocation` "/Game/AUDIO/SFX_Weapons/Weap_GrenadeLauncher/SC_Explosion.SC_Explosion" _returnvalue (struct) 1.0 1.0 0.0 null null null)
      (`GameplayStatics.SpawnEmitterAtLocation` "/Game/kosm_fps_assets/Misc/Particles/P_Explode2.P_Explode2" _returnvalue (struct) (4.0 4.0 4.0))
      (bind _returnvalue_2 (`GameplayStatics.SpawnEmitterAtLocation` "/Game/StylizedNatureVol2/Effects/P_Fog_Cloud.P_Fog_Cloud" _returnvalue (struct) (2.0 2.0 2.0)))
      (`ActorComponent.K2_DestroyComponent` (`self.Niagara`))
      (`ActorComponent.K2_DestroyComponent` (`self.ParticleSystem1`))
      (`KismetSystemLibrary.Delay` 6.0)
      (`ActorComponent.K2_DestroyComponent` _returnvalue_2)
      (`self.K2_DestroyActor`))))

(event `self.ProjectileMovement.OnProjectileBounce`
  (params (ImpactResult :type "HitResult Structure (by ref)") (ImpactVelocity :type "Vector Structure (by ref)"))
  (`GameplayStatics.PlaySoundAtLocation` "/Game/AUDIO/SFX_Weapons/Weap_GrenadeLauncher/SC_GrenadeHit.SC_GrenadeHit" (`self.K2_GetActorLocation`) (struct) 1.5 2.0 0.0 null null null))

(fn `UserConstructionScript`)