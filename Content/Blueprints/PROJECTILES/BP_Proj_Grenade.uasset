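; Grenade projectile that explodes on a hit or when its sphere overlaps anything but the instigator, with a sound on bounces.
; Hits on non-movable components also leave a temporary crater decal.
; The blast applies radial damage, ignoring "Red Team" tagged actors plus the player pawn in team mode.
; It also fires a radial impulse, spawns effects, sound and camera shake, then hides and destroys itself after a short delay.
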(event `self.ReceiveHit`
  (params (MyComp :type "PrimitiveComponent Object Reference") (Other :type "Actor Object Reference") (OtherComp :type "PrimitiveComponent Object Reference") (bSelfMoved :type Boolean) (HitLocation :type "Vector Structure") (HitNormal :type "Vector Structure") (NormalImpulse :type "Vector Structure") (Hit :type "HitResult Structure (by ref)"))
  (bind _returnvalue (`self.K2_GetActorLocation`))
  (bind _radialforce (`self.RadialForce`))
  (if (`|EnumInequality` (`SceneComponent.Mobility` OtherComp) "Movable")
    (`/Engine/EditorBlueprintResources/StandardMacros.IsValid` OtherComp
      (:`Is Valid`
        (bind _returnvalue_2 (`GameplayStatics.SpawnDecalAttached` "/Game/kosm_fps_assets/Misc/Materials/D_Crater.D_Crater" (100.0 100.0 100.0) OtherComp "None" (`KismetMathLibrary.InverseTransformLocation` (`SceneComponent.K2_GetComponentToWorld` OtherComp) HitLocation) (`KismetMathLibrary.Conv_VectorToRotator` HitNormal) "KeepRelativeOffset" 30.0))
        (`/Engine/EditorBlueprintResources/StandardMacros.IsValid` _returnvalue_2
          (:`Is Valid`
            (`DecalComponent.SetFadeScreenSize` _returnvalue_2 0.001))
          (:`Is Not Valid`
            _)))
      (:`Is Not Valid`
        _)))
  (`GameplayStatics.SpawnEmitterAtLocation` "/Game/kosm_fps_assets/Misc/Particles/P_Explode1.P_Explode1" (`self.K2_GetActorLocation`) (struct) (5.0 5.0 5.0) :!label _label)
  (bind _outactors (`GameplayStatics.GetAllActorsWithTag` "Red Team"))
  (bind _game_instance (`/Game/Blueprints/NewFunctionLibrary.dead game instance`))
  (if (`/Game/Blueprints/DeadGaemInstance.team mode?` _game_instance)
    (`KismetArrayLibrary.Array_Append` _outactors (`|MakeArray` (`GameplayStatics.GetPlayerPawn` 0) :!type "Actor Object Reference")))
  (`GameplayStatics.ApplyRadialDamage` 75.0 _returnvalue 1200.0 null _outactors self (`self.GetInstigatorController`))
  (`/Engine/EditorBlueprintResources/StandardMacros.IsValid` _radialforce
    (:`Is Valid`
      (`RadialForceComponent.FireImpulse` _radialforce)
      (`ActorComponent.K2_DestroyComponent` (`self.RadialForce`)))
    (:`Is Not Valid`
      _))
  (`SceneComponent.SetHiddenInGame` (`self.StaticMesh`) true false)
  (`self.SetActorEnableCollision` false)
  (`GameplayStatics.PlaySoundAtLocation` "/Game/AUDIO/SFX_Weapons/Weap_GrenadeLauncher/SC_Explosion.SC_Explosion" _returnvalue (struct) 1.0 1.0 0.0 null null null)
  (`GameplayStatics.PlayWorldCameraShake` "/Game/Blueprints/SHAKES/BP_CameraShake_Jump_Heavy.BP_CameraShake_Jump_Heavy_C" _returnvalue 900.0 2000.0 0.5)
  (`KismetSystemLibrary.Delay` 0.3)
  (`self.K2_DestroyActor`))

(event `self.Sphere.OnComponentBeginOverlap`
  (params (OverlappedComponent :type "PrimitiveComponent Object Reference") (OtherActor :type "Actor Object Reference") (OtherComp :type "PrimitiveComponent Object Reference") (OtherBodyIndex :type Integer) (bFromSweep :type Boolean) (SweepResult :type "HitResult Structure (by ref)"))
  (if (!= OtherActor (`self.GetInstigator`))
    (goto _label)))

(event `self.ProjectileMovement.OnProjectileBounce`
  (params (ImpactResult :type "HitResult Structure (by ref)") (ImpactVelocity :type "Vector Structure (by ref)"))
  (`GameplayStatics.PlaySoundAtLocation` "/Game/AUDIO/SFX_Weapons/Weap_GrenadeLauncher/SC_GrenadeHit.SC_GrenadeHit" (`self.K2_GetActorLocation`) (struct) 1.0 1.0 0.0 null null null))

(fn `UserConstructionScript`)