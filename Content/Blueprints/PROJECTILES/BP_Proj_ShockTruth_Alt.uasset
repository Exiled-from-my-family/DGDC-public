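; Alt-fire projectile for the ShockTruth weapon that draws a lightning beam from the shooter's muzzle to its impact point.
; BeginPlay sets the beam source from player or bot instigators, then destroys non-authority copies; construction makes collision ignore the instigator.
; The first hit applies tiny-radius damage, spawns lightning, bullet-hole and blood effects, and sets the beam end.
; Hitting a power terminal calls DAMAGED on the first terminal found by class.
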(event `self.ReceiveBeginPlay`
  (bind _returnvalue (`self.GetInstigator`))
  (bind _particlesystem (`self.ParticleSystem`))
  (bind (_asfps_movement_character_light_1_vq_3 _bsuccess) (cast `/Game/Blueprints/CHARACTERS/fpsMovementCharacter_light_1_vq3` _returnvalue :!pure true))
  (bind (_asfps_movement_character_light_2_cpma _bsuccess_2) (cast `/Game/Blueprints/CHARACTERS/fpsMovementCharacter_light_2_cpma` _returnvalue :!pure true))
  (if _bsuccess
    (`ParticleSystemComponent.SetBeamSourcePoint` (`self.ParticleSystem`) 0 (`SceneComponent.K2_GetComponentLocation` (`/Game/Blueprints/CHARACTERS/fpsMovementCharacter_light_1_vq3.Muzzle1P` _asfps_movement_character_light_1_vq_3)) 0)
    (elif _bsuccess_2
      (`ParticleSystemComponent.SetBeamSourcePoint` _particlesystem 0 (`SceneComponent.K2_GetComponentLocation` (`/Game/Blueprints/CHARACTERS/fpsMovementCharacter_light_2_cpma.Muzzle1P` _asfps_movement_character_light_2_cpma)) 0)
      (else
        (bind _asai_noobot_char (cast `/Game/Blueprints/CHARACTERS/NoobotAI/Blueprints/AI_NoobotChar` _returnvalue))
        (`ParticleSystemComponent.SetBeamSourcePoint` _particlesystem 0 (`SceneComponent.K2_GetComponentLocation` (`/Game/Blueprints/CHARACTERS/NoobotAI/Blueprints/AI_NoobotChar.WeaponMuzzle` _asai_noobot_char)) 0))))
  (`/Engine/EditorBlueprintResources/ActorMacros.Switch Has Authority`
    (:`Remote`
      (`self.K2_DestroyActor`))))

(event `self.ReceiveHit`
  (params (MyComp :type "PrimitiveComponent Object Reference") (Other :type "Actor Object Reference") (OtherComp :type "PrimitiveComponent Object Reference") (bSelfMoved :type Boolean) (HitLocation :type "Vector Structure") (HitNormal :type "Vector Structure") (NormalImpulse :type "Vector Structure") (Hit :type "HitResult Structure (by ref)"))
  (bind (_bblockinghit _binitialoverlap _time _distance _location _impactpoint _normal _impactnormal _physmat _hitactor _hitcomponent _hitbonename) (`GameplayStatics.BreakHitResult` Hit))
  (bind _returnvalue (`self.K2_GetActorLocation`))
  (bind _returnvalue_2 (`KismetMathLibrary.Conv_VectorToRotator` _normal))
  (bind _returnvalue_3 (`KismetMathLibrary.MakeTransform` (0.0 0.0 0.0) _returnvalue_2))
  ;[0.3687 0.5739 1] Begin Play / Apply Damage / Event Hit / Line Trace
  (`/Engine/EditorBlueprintResources/StandardMacros.DoOnce` false
    (:`Completed`
      (`GameplayStatics.ApplyRadialDamage` :`BaseDamage` 12.0 :`Origin` HitLocation :`DamageRadius` 1.0 :`DamageCauser` self :`InstigatedByController` (`self.GetInstigatorController`) :`bDoFullDamage` true)
      (`GameplayStatics.SpawnEmitterAtLocation` "/Game/kosm_fps_assets/Misc/Particles/P_Lightning.P_Lightning" _returnvalue (struct) (2.0 2.0 2.0))
      (`ParticleSystemComponent.SetBeamTargetPoint` (`self.ParticleSystem`) 0 _returnvalue 0)
      (`/Engine/EditorBlueprintResources/StandardMacros.IsValid` _hitactor
        (:`Is Valid`
          (if (not (`self.ActorHasTag` _hitactor "Projectile"))
            (bind _returnvalue_4 (`GameplayStatics.SpawnDecalAttached` "/Game/kosm_fps_assets/Misc/Materials/BulletHole001.BulletHole001" (10.0 10.0 10.0) OtherComp "None" (`KismetMathLibrary.InverseTransformLocation` (`SceneComponent.K2_GetComponentToWorld` OtherComp) HitLocation) _returnvalue_2 "KeepRelativeOffset" 30.0))
            (`/Engine/EditorBlueprintResources/StandardMacros.IsValid` _returnvalue_4
              (:`Is Valid`
                (`DecalComponent.SetFadeScreenSize` _returnvalue_4 0.001))
              (:`Is Not Valid`
                _)))
          (if (`.bSuccess` (cast `Character` _hitactor :!pure true))
            (bind _returnvalue_5 (`GameplayStatics.SpawnDecalAtLocation` "/Game/kosm_fps_assets/Misc/Materials/D_BloodStain.D_BloodStain" (`KismetMathLibrary.MakeVector` (`KismetMathLibrary.RandomFloatInRange` 5.0 30.0) (`KismetMathLibrary.RandomFloatInRange` 5.0 30.0) (`KismetMathLibrary.RandomFloatInRange` 5.0 30.0)) _location (`KismetMathLibrary.MakeRotator` (`KismetMathLibrary.RandomFloatInRange` (.roll (.rotation _returnvalue_3)) 360.0) (.pitch (.rotation _returnvalue_3)) (.yaw (.rotation _returnvalue_3)))))
            (`SceneComponent.K2_AttachToComponent` _returnvalue_5 _hitcomponent _hitbonename "KeepWorld" "KeepWorld" "KeepWorld" true)
            (`DecalComponent.SetFadeScreenSize` _returnvalue_5 0.001)
            (`GameplayStatics.SpawnEmitterAttached` "/Game/kosm_fps_assets/Misc/Particles/PS_Blood_BulletHit.PS_Blood_BulletHit" _hitcomponent "None" (`KismetMathLibrary.InverseTransformLocation` (`SceneComponent.K2_GetComponentToWorld` _hitcomponent) _location) _returnvalue_2 (0.5 0.5 0.5)))
          ;;[1 1 1] if it hits the terminal then the event is fired on that actor's end
          (if (`.bSuccess` (cast `/Game/MISSIONS/EP3/Blueprints/BP_Power_Terminal` _hitactor :!pure true))
            (bind _returnvalue_6 (`GameplayStatics.GetActorOfClass` "/Game/MISSIONS/EP3/Blueprints/BP_Power_Terminal.BP_Power_Terminal_C"))
            (`/Game/MISSIONS/EP3/Blueprints/BP_Power_Terminal.DAMAGED` _returnvalue_6))
          (`KismetSystemLibrary.Delay` 1.0)
          (`self.K2_DestroyActor`))
        (:`Is Not Valid`)))))

(fn `IgnoreActorWhenMoving`
  (`PrimitiveComponent.IgnoreActorWhenMoving` (`self.CollisionComponent`) (`self.GetInstigator`) true))

(fn `UserConstructionScript`
  (`self.IgnoreActorWhenMoving`))