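; Shock rifle projectile that draws a beam from the instigator's muzzle and detonates shock orbs in combos.
; BeginPlay sets the beam source, destroys remote copies, and sphere-traces forward for a BP_Proj_Orb, triggering radial damage, impulse and burst effects if found.
; The first hit applies point-like damage, ends the beam there unless a combo occurred, and adds impact decals and blood.
; Eligible non-flying ep1_character targets get launched upward, then along the shot direction.
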(event `self.ReceiveBeginPlay`
  (bind _returnvalue (`self.GetInstigator`))
  (bind _returnvalue_2 (`self.K2_GetActorLocation`))
  (bind _particlesystem (`self.ParticleSystem`))
  (bind (_asfps_movement_character_light_1_vq_3 _bsuccess) (cast `/Game/Blueprints/CHARACTERS/fpsMovementCharacter_light_1_vq3` _returnvalue :!pure true))
  (bind (_asfps_movement_character_light_2_cpma _bsuccess_2) (cast `/Game/Blueprints/CHARACTERS/fpsMovementCharacter_light_2_cpma` _returnvalue :!pure true))
  (`|ExecutionSequence`
    (:`then_0`
      (if _bsuccess
        (`ParticleSystemComponent.SetBeamSourcePoint` (`self.ParticleSystem`) 0 (`SceneComponent.K2_GetComponentLocation` (`/Game/Blueprints/CHARACTERS/fpsMovementCharacter_light_1_vq3.Muzzle1P` _asfps_movement_character_light_1_vq_3)) 0)
        (elif _bsuccess_2
          (`ParticleSystemComponent.SetBeamSourcePoint` _particlesystem 0 (`SceneComponent.K2_GetComponentLocation` (`/Game/Blueprints/CHARACTERS/fpsMovementCharacter_light_2_cpma.Muzzle1P` _asfps_movement_character_light_2_cpma)) 0)
          (else
            (bind _asai_noobot_char (cast `/Game/Blueprints/CHARACTERS/NoobotAI/Blueprints/AI_NoobotChar` _returnvalue))
            (`ParticleSystemComponent.SetBeamSourcePoint` _particlesystem 0 (`SceneComponent.K2_GetComponentLocation` (`/Game/Blueprints/CHARACTERS/NoobotAI/Blueprints/AI_NoobotChar.WeaponMuzzle` _asai_noobot_char)) 0))))
      (`/Engine/EditorBlueprintResources/ActorMacros.Switch Has Authority`
        (:`Remote`
          (`self.K2_DestroyActor`))))
    (:`then_1`
      ;[0.2985 0.1661 1] ORB COMBO code
      (bind _outhit (`KismetSystemLibrary.SphereTraceSingle` _returnvalue_2 (+ _returnvalue_2 (* (`self.GetActorForwardVector`) 100000.0)) 16.0 "TraceTypeQuery1"))
      (bind (_bblockinghit _binitialoverlap _time _distance _location _impactpoint _normal _impactnormal _physmat _hitactor) (`GameplayStatics.BreakHitResult` _outhit))
      (bind (_asbp_proj_orb _bsuccess_3) (cast `/Game/Blueprints/PROJECTILES/BP_Proj_Orb` _hitactor :!pure true))
      (if _bsuccess_3
        (set `self.Shocked` true)
        (`self.K2_DestroyActor` _asbp_proj_orb)
        (`ParticleSystemComponent.SetBeamTargetPoint` (`self.ParticleSystem`) 0 _impactpoint 0)
        (`|SpawnActorFromClass` "/Game/Blueprints/PROJECTILES/BP_HitBurst.BP_HitBurst_C" (`KismetMathLibrary.MakeTransform` _impactpoint) "Undefined" "OverrideRootScale" null (0.25 0.0 1.0) null)
        (bind _returnvalue_3 (`KismetMathLibrary.MakeTransform` _impactpoint (struct) (0.75 0.75 0.75)))
        (`|SpawnActorFromClass` "/Game/Blueprints/PROJECTILES/BP_SonicBurst.BP_SonicBurst_C" _returnvalue_3 "Undefined" "OverrideRootScale" null null)
        (`GameplayStatics.SpawnEmitterAtLocation` "/Game/kosm_fps_assets/Misc/Particles/P_BubbleBurst1_1.P_BubbleBurst1_1" _impactpoint (struct) (20.0 20.0 20.0))
        (`GameplayStatics.SpawnEmitterAtLocation` "/Game/kosm_fps_assets/Misc/Particles/P_BubbleBurst2.P_BubbleBurst2" _impactpoint (struct) (4.0 4.0 4.0))
        (bind _player (`/Game/Blueprints/NewFunctionLibrary.get player`))
        (bind _returnvalue_4 (`AddComponent|NODE_AddRadialForceComponent-0` :`RelativeTransform` _returnvalue_3))
        (set `RadialForceComponent.Radius` 400.0 _returnvalue_4)
        (set `RadialForceComponent.ImpulseStrength` 2400.0 _returnvalue_4)
        (set `RadialForceComponent.bImpulseVelChange` true _returnvalue_4)
        (`RadialForceComponent.FireImpulse` _returnvalue_4)
        (`GameplayStatics.ApplyRadialDamage` 200.0 _impactpoint 1250.0 null (`|MakeArray` _player :!type "Actor Object Reference") null null)
        (`GameplayStatics.PlaySoundAtLocation` "/Game/AUDIO/SFX_Weapons/Weap_ShockRifle/SC_ShockExplosion.SC_ShockExplosion" _impactpoint (struct) 1.0 1.0 0.0 null null null)
        (`PlayerCameraManager.PlayCameraShake` :`self` (`GameplayStatics.GetPlayerCameraManager` 0) :`ShakeClass` "/Game/Blueprints/SHAKES/BP_CameraShake_Jump_Heavy.BP_CameraShake_Jump_Heavy_C" :`Scale` 2.0)
        (`KismetSystemLibrary.Delay` 0.5)
        (`self.K2_DestroyActor`)))))

(event `self.ReceiveHit`
  (params (MyComp :type "PrimitiveComponent Object Reference") (Other :type "Actor Object Reference") (OtherComp :type "PrimitiveComponent Object Reference") (bSelfMoved :type Boolean) (HitLocation :type "Vector Structure") (HitNormal :type "Vector Structure") (NormalImpulse :type "Vector Structure") (Hit :type "HitResult Structure (by ref)"))
  (bind (_bblockinghit _binitialoverlap _time _distance _location _impactpoint _normal _impactnormal _physmat _hitactor _hitcomponent _hitbonename) (`GameplayStatics.BreakHitResult` Hit))
  (bind _returnvalue (`self.K2_GetActorLocation`))
  (bind _returnvalue_2 (`KismetMathLibrary.Conv_VectorToRotator` _normal))
  (bind (_asep_1_character _bsuccess) (cast `/Game/MISSIONS/EP1/Characters/ep1_character` _hitactor :!pure true))
  (bind _returnvalue_3 (`KismetMathLibrary.MakeTransform` (0.0 0.0 0.0) _returnvalue_2))
  ;[0.3687 0.5739 1] Begin Play / Apply Damage / Event Hit / Line Trace
  (`/Engine/EditorBlueprintResources/StandardMacros.DoOnce` false
    (:`Completed`
      (`|ExecutionSequence`
        (:`then_0`
          (`GameplayStatics.ApplyRadialDamage` :`BaseDamage` 36.0 :`Origin` HitLocation :`DamageRadius` 1.0 :`DamageCauser` self :`InstigatedByController` (`self.GetInstigatorController`) :`bDoFullDamage` true)
          (`GameplayStatics.SpawnEmitterAtLocation` "/Game/kosm_fps_assets/Misc/Particles/P_Lightning.P_Lightning" _returnvalue (struct) (2.0 2.0 2.0))
          (`|SpawnActorFromClass` "/Game/Blueprints/PROJECTILES/BP_HitBurst.BP_HitBurst_C" (`KismetMathLibrary.MakeTransform` _returnvalue (struct) (0.25 0.25 0.25)) "Undefined" "OverrideRootScale" null (0.25 0.0 1.0) null)
          (if (not (`self.Shocked`))
            (`ParticleSystemComponent.SetBeamTargetPoint` (`self.ParticleSystem`) 0 _returnvalue 0))
          (`/Engine/EditorBlueprintResources/StandardMacros.IsValid` _hitactor
            (:`Is Valid`
              (if (not (`self.ActorHasTag` _hitactor "Projectile"))
                (bind _returnvalue_4 (`GameplayStatics.SpawnDecalAttached` "/Game/kosm_fps_assets/Misc/Materials/BulletHole001.BulletHole001" (10.0 10.0 10.0) OtherComp "None" (`KismetMathLibrary.InverseTransformLocation` (`SceneComponent.K2_GetComponentToWorld` OtherComp) HitLocation) _returnvalue_2 "KeepRelativeOffset" 30.0))
                (`/Engine/EditorBlueprintResources/StandardMacros.IsValid` _returnvalue_4
                  (:`Is Valid`
                    (`DecalComponent.SetFadeScreenSize` _returnvalue_4 0.001))
                  (:`Is Not Valid`
                    _)))
              (if (`.bSuccess` (cast `Character` _hitactor :!pure true))
                (bind _returnvalue_5 (`GameplayStatics.SpawnDecalAtLocation` "/Game/kosm_fps_assets/Misc/Materials/D_BloodStain.D_BloodStain" (`KismetMathLibrary.MakeVector` (`KismetMathLibrary.RandomFloatInRange` 5.0 30.0) (`KismetMathLibrary.RandomFloatInRange` 5.0 30.0) (`KismetMathLibrary.RandomFloatInRange` 5.0 30.0)) _location (`KismetMathLibrary.MakeRotator` (`KismetMathLibrary.RandomFloatInRange` (.roll (.rotation _returnvalue_3)) 360.0) (.pitch (.rotation _returnvalue_3)) (.yaw (.rotation _returnvalue_3)))))
                (`SceneComponent.K2_AttachToComponent` _returnvalue_5 _hitcomponent _hitbonename "KeepWorld" "KeepWorld" "KeepWorld" true)
                (`DecalComponent.SetFadeScreenSize` _returnvalue_5 0.001)
                (`GameplayStatics.SpawnEmitterAttached` "/Game/kosm_fps_assets/Misc/Particles/PS_Blood_BulletHit.PS_Blood_BulletHit" _hitcomponent "None" (`KismetMathLibrary.InverseTransformLocation` (`SceneComponent.K2_GetComponentToWorld` _hitcomponent) _location) _returnvalue_2 (0.5 0.5 0.5)))
              (`KismetSystemLibrary.Delay` 1.0)
              (`self.K2_DestroyActor`))))
        (:`then_1`
          (if (and _bsuccess (not (`NavMovementComponent.IsFlying` (`Character.CharacterMovement` _asep_1_character))) (not (or (`self.ActorHasTag` _hitactor "Ghost") (`self.ActorHasTag` _hitactor "Molly") (`self.ActorHasTag` _hitactor "TooBig"))))
            (`Character.LaunchCharacter` _asep_1_character (0.0 0.0 1000.0) false false)
            (`KismetSystemLibrary.Delay` 0.1)
            (`Character.LaunchCharacter` _asep_1_character (* (`self.GetActorForwardVector`) 1500.0) true false)))))))

(fn `IgnoreActorWhenMoving`
  (`PrimitiveComponent.IgnoreActorWhenMoving` (`self.CollisionComponent`) (`self.GetInstigator`) true))

(fn `UserConstructionScript`
  (`self.IgnoreActorWhenMoving`))