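; Shotgun pellet projectile that launches at high speed with random spread, ignoring collision with its instigator.
; On spawn it traces forward, disables physics simulation unless a PortalBP is hit, and enables CCD shortly after.
; Its first hit deals small-radius damage sparing Red Team, with impact effects and sound.
; Movable surfaces get blood effects if an Undead tag check passes, others get craters, then the pellet hides and is destroyed.
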(event `self.ReceiveBeginPlay`
  (bind _projectile (`self.Projectile`))
  (bind _spread (`self.Spread`))
  (bind _collisioncomponent (`self.CollisionComponent`))
  (bind _returnvalue (`SceneComponent.K2_GetComponentLocation` _collisioncomponent))
  (bind _returnvalue_2 (/ _spread 2.0))
  ;[0.3687 0.5739 1] Begin Play / Apply Damage / Event Hit / Line Trace
  (`ProjectileMovementComponent.SetVelocityInLocalSpace` _projectile (`KismetMathLibrary.MakeVector` 100000.0 (`KismetMathLibrary.RandomFloatInRange` _spread (* _spread -1.0)) (`KismetMathLibrary.RandomFloatInRange` _returnvalue_2 (* _returnvalue_2 -1.0))))
  (set `ProjectileMovementComponent.bRotationFollowsVelocity` true _projectile)
  (`|ExecutionSequence`
    (:`then_0`
      (bind _outactors (`GameplayStatics.GetAllActorsWithTag` "Character"))
      (bind _outactors_2 (`GameplayStatics.GetAllActorsWithTag` "Projectile"))
      (`KismetArrayLibrary.Array_Append` _outactors_2 _outactors)
      (bind _outhit (`KismetSystemLibrary.LineTraceSingle` _returnvalue (+ _returnvalue (* (`KismetMathLibrary.GetForwardVector` (`SceneComponent.K2_GetComponentRotation` _collisioncomponent)) 100000.0)) "TraceTypeQuery1" false _outactors_2))
      (if (not (`.bSuccess` (cast `/Game/kosm_fps_assets/Misc/Portal/PortalBP` (`.HitActor` (`GameplayStatics.BreakHitResult` _outhit)) :!pure true)))
        (`PrimitiveComponent.SetSimulatePhysics` (`self.CollisionComponent`) false)))
    (:`then_1`
      (`KismetSystemLibrary.Delay` 0.02)
      (`PrimitiveComponent.SetUseCCD` (`self.CollisionComponent`) true "None"))))

(event `self.ReceiveHit`
  (params (MyComp :type "PrimitiveComponent Object Reference") (Other :type "Actor Object Reference") (OtherComp :type "PrimitiveComponent Object Reference") (bSelfMoved :type Boolean) (HitLocation :type "Vector Structure") (HitNormal :type "Vector Structure") (NormalImpulse :type "Vector Structure") (Hit :type "HitResult Structure (by ref)"))
  (bind _returnvalue (`KismetMathLibrary.Conv_VectorToRotator` (`.Normal` (`GameplayStatics.BreakHitResult` Hit))))
  ;[0.3687 0.5739 1] Begin Play / Apply Damage / Event Hit / Line Trace
  (`/Engine/EditorBlueprintResources/StandardMacros.DoOnce` false
    (:`Completed`
      (bind _outactors (`GameplayStatics.GetAllActorsWithTag` "Red Team"))
      (`GameplayStatics.ApplyRadialDamage` 9.0 HitLocation 5.0 null _outactors self (`self.GetInstigatorController`) true)
      (`GameplayStatics.SpawnEmitterAtLocation` "/Game/kosm_fps_assets/Misc/Particles/P_Pellet_Impact.P_Pellet_Impact" (`self.K2_GetActorLocation`) (struct) (8.0 8.0 8.0))
      (`GameplayStatics.PlaySoundAtLocation` "/Game/AUDIO/SFX_Weapons/Weap_Nailgun/SC_Nailgun_Ricochet.SC_Nailgun_Ricochet" (`SceneComponent.K2_GetComponentLocation` (`self.RadialForce`)) (struct) 0.75 1.0 0.0 null null null)
      (`/Engine/EditorBlueprintResources/StandardMacros.IsValid` null
        (:`Is Valid`
          _)
        (:`Is Not Valid`
          _))
      (if (`|EnumEquality` (`SceneComponent.Mobility` OtherComp) "Movable")
        (if (`self.ActorHasTag` "Undead")
          (bind (_outhit _returnvalue_2) (`KismetSystemLibrary.LineTraceSingle` HitLocation (+ HitLocation (* (`KismetMathLibrary.GetUpVector` (`KismetMathLibrary.FindLookAtRotation` (`self.K2_GetActorLocation`) HitLocation)) -300.0)) "TraceTypeQuery1"))
          (if _returnvalue_2
            (bind (_bblockinghit _binitialoverlap _time _distance _location _impactpoint _normal) (`GameplayStatics.BreakHitResult` _outhit))
            (bind _returnvalue_3 (`GameplayStatics.SpawnDecalAtLocation` (select `int` (`KismetMathLibrary.RandomIntegerInRange` 0 7) :`0` "/Game/kosm_fps_assets/Misc/Materials/D_BloodStain_Inst.D_BloodStain_Inst" :`1` "/Game/kosm_fps_assets/Misc/Materials/D_BloodStain_Inst1.D_BloodStain_Inst1" :`2` "/Game/kosm_fps_assets/Misc/Materials/D_BloodStain_Inst2.D_BloodStain_Inst2" :`3` "/Game/kosm_fps_assets/Misc/Materials/D_BloodStain_Inst3.D_BloodStain_Inst3" :`4` "/Game/kosm_fps_assets/Misc/Materials/D_BloodStain_Inst4.D_BloodStain_Inst4" :`5` "/Game/kosm_fps_assets/Misc/Materials/D_BloodStain_Inst5.D_BloodStain_Inst5" :`6` "/Game/kosm_fps_assets/Misc/Materials/D_BloodStain_Inst6.D_BloodStain_Inst6" :`7` "/Game/kosm_fps_assets/Misc/Materials/D_BloodStain_Inst7.D_BloodStain_Inst7" :!type "MaterialInterface Object Reference") (`KismetMathLibrary.MakeVector` (`KismetMathLibrary.RandomFloatInRange` 120.0 150.0) (`KismetMathLibrary.RandomFloatInRange` 120.0 150.0) (`KismetMathLibrary.RandomFloatInRange` 120.0 150.0)) _location (`KismetMathLibrary.MakeRotFromX` _normal) 10.0))
            (`DecalComponent.SetFadeScreenSize` _returnvalue_3 0.001))
          (`GameplayStatics.SpawnEmitterAttached` "/Game/kosm_fps_assets/Misc/Particles/PS_Blood_BulletHit1.PS_Blood_BulletHit1" null "None" (0.0 0.0 0.0) _returnvalue (0.75 0.75 0.75)))
        (else
          (bind _returnvalue_4 (`GameplayStatics.SpawnDecalAttached` "/Game/kosm_fps_assets/Misc/Materials/D_Crater.D_Crater" (10.0 10.0 10.0) OtherComp "None" (`KismetMathLibrary.InverseTransformLocation` (`SceneComponent.K2_GetComponentToWorld` OtherComp) HitLocation) _returnvalue "SnapToTargetIncludingScale" 5.0))
          (`/Engine/EditorBlueprintResources/StandardMacros.IsValid` _returnvalue_4
            (:`Is Valid`
              (`DecalComponent.SetFadeScreenSize` _returnvalue_4 0.001))
            (:`Is Not Valid`
              _))))
      (`SceneComponent.ToggleVisibility` (`self.Pellet`) false)
      (`KismetSystemLibrary.Delay` 2.0)
      (`self.K2_DestroyActor`))))

(fn `IgnoreActorWhenMoving`
  (`PrimitiveComponent.IgnoreActorWhenMoving` (`self.CollisionComponent`) (`self.GetInstigator`) true))

(fn `UserConstructionScript`
  (`self.IgnoreActorWhenMoving`))