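; Charged alt-fire laser gun projectile whose DamageCharge sets its size, radial damage, blast radius, hit-burst scale and camera shake.
; On spawn it pins a beam to the instigator's first-person muzzle, destroying itself on remotes or without that character type.
; On hit it ends the beam there, damages and spawns effects, then on valid actors adds crater decals to non-projectiles and self-destroys after a delay.
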(event `self.ReceiveBeginPlay`
  (bind _damage_charge (`self.Damage_Charge`))
  (bind (_asfps_movement_character_light_1_vq_3 _bsuccess) (cast `/Game/Blueprints/CHARACTERS/fpsMovementCharacter_light_1_vq3` (`self.GetInstigator`) :!pure true))
  (`KismetSystemLibrary.PrintString` (`KismetStringLibrary.Concat_StrStr` "charge amt: " (`KismetStringLibrary.Conv_DoubleToString` _damage_charge)) true false)
  (`self.SetActorScale3D` (`KismetMathLibrary.Conv_DoubleToVector` (`KismetMathLibrary.FClamp` (`KismetMathLibrary.SafeDivide` (* _damage_charge 2.0) 50.0) 0.25 2.0)))
  (if _bsuccess
    (`ParticleSystemComponent.SetBeamSourcePoint` (`self.ParticleSystem`) 0 (`SceneComponent.K2_GetComponentLocation` (`/Game/Blueprints/CHARACTERS/fpsMovementCharacter_light_1_vq3.Muzzle1P` _asfps_movement_character_light_1_vq_3)) 0)
    (`/Engine/EditorBlueprintResources/ActorMacros.Switch Has Authority`
      (:`Remote`
        (`self.K2_DestroyActor`)))
    (else
      (`self.K2_DestroyActor`))))

(event `self.ReceiveHit`
  (params (MyComp :type "PrimitiveComponent Object Reference") (Other :type "Actor Object Reference") (OtherComp :type "PrimitiveComponent Object Reference") (bSelfMoved :type Boolean) (HitLocation :type "Vector Structure") (HitNormal :type "Vector Structure") (NormalImpulse :type "Vector Structure") (Hit :type "HitResult Structure (by ref)"))
  (bind (_bblockinghit _binitialoverlap _time _distance _location _impactpoint _normal _impactnormal _physmat _hitactor) (`GameplayStatics.BreakHitResult` Hit))
  (bind _returnvalue (`self.K2_GetActorLocation`))
  (bind _returnvalue_2 (`self.GetInstigatorController`))
  (bind _damage_charge (`self.Damage_Charge`))
  (bind _returnvalue_3 (`KismetMathLibrary.SafeDivide` (* (`self.Damage_Charge`) 2.0) 100.0))
  ;[0.3687 0.5739 1] Begin Play / Apply Damage / Event Hit / Line Trace
  (`GameplayStatics.ApplyRadialDamage` (* _damage_charge 1.5) (`self.K2_GetActorLocation`) (* _damage_charge 15.0) null (`|MakeArray` _returnvalue_2 (`GameplayStatics.GetPlayerCharacter` 0) :!type "Actor Object Reference") self _returnvalue_2 false "ECC_GameTraceChannel1")
  (`GameplayStatics.SpawnEmitterAtLocation` "/Game/kosm_fps_assets/Misc/Particles/P_RailgunBurst1.P_RailgunBurst1" HitLocation (struct) (6.0 6.0 6.0))
  (`ParticleSystemComponent.SetBeamTargetPoint` (`self.ParticleSystem`) 0 _returnvalue 0)
  (`|SpawnActorFromClass` "/Game/Blueprints/PROJECTILES/BP_HitBurst.BP_HitBurst_C" (`KismetMathLibrary.MakeTransform` _returnvalue (struct) (* (1.0 1.0 1.0) (`KismetMathLibrary.FClamp` _returnvalue_3 0.1))) "Undefined" "OverrideRootScale" null (1.0 0.1 0.0) null)
  (`PlayerCameraManager.PlayCameraShake` :`self` (`GameplayStatics.GetPlayerCameraManager` 0) :`ShakeClass` "/Game/Blueprints/SHAKES/BP_CameraShake_Explosion.BP_CameraShake_Explosion_C" :`Scale` (`KismetMathLibrary.FClamp` (* _returnvalue_3 2.0) 0.1 2.0))
  (`/Engine/EditorBlueprintResources/StandardMacros.IsValid` _hitactor
    (:`Is Valid`
      (if (not (`self.ActorHasTag` _hitactor "Projectile"))
        (bind _returnvalue_4 (`GameplayStatics.SpawnDecalAttached` "/Game/kosm_fps_assets/Misc/Materials/D_Crater.D_Crater" (6.0 6.0 6.0) OtherComp "None" (`KismetMathLibrary.InverseTransformLocation` (`SceneComponent.K2_GetComponentToWorld` OtherComp) HitLocation) (`KismetMathLibrary.Conv_VectorToRotator` _normal) "KeepRelativeOffset" 30.0))
        (`/Engine/EditorBlueprintResources/StandardMacros.IsValid` _returnvalue_4
          (:`Is Valid`
            (`DecalComponent.SetFadeScreenSize` _returnvalue_4 0.001))
          (:`Is Not Valid`
            _)))
      (`KismetSystemLibrary.Delay` 0.5)
      (`self.K2_DestroyActor`))))

(fn `IgnoreActorWhenMoving`
  (`PrimitiveComponent.IgnoreActorWhenMoving` (`self.CollisionComponent`) (`self.GetInstigator`) true))

(fn `UserConstructionScript`
  (`self.IgnoreActorWhenMoving`))