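; Alt-fire Ice Gun projectile that bounces with a sound and explodes into an ice burst with radial damage.
; Hit runs once and adds a crater decal on non-movable surfaces; Sphere overlap with anyone but the instigator jumps straight to detonation, bypassing the DoOnce.
; Detonation spawns effects and burst actors, hides the projectile, then destroys it and the decal after a short delay.
; The nearby-character slow trace is disconnected.
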(event `self.ReceiveHit`
  (params (MyComp :type "PrimitiveComponent Object Reference") (Other :type "Actor Object Reference") (OtherComp :type "PrimitiveComponent Object Reference") (bSelfMoved :type Boolean) (HitLocation :type "Vector Structure") (HitNormal :type "Vector Structure") (NormalImpulse :type "Vector Structure") (Hit :type "HitResult Structure (by ref)"))
  (bind _returnvalue (`self.GetInstigator`))
  (bind _returnvalue_2 (`self.K2_GetActorLocation`))
  (`/Engine/EditorBlueprintResources/StandardMacros.DoOnce` false
    (:`Completed`
      (if (`|EnumInequality` (`SceneComponent.Mobility` OtherComp) "Movable")
        (`/Engine/EditorBlueprintResources/StandardMacros.IsValid` OtherComp
          (:`Is Valid`
            (bind _returnvalue_3 (`GameplayStatics.SpawnDecalAttached` "/Game/kosm_fps_assets/Misc/Materials/D_Crater.D_Crater" (100.0 100.0 100.0) OtherComp "None" (`KismetMathLibrary.InverseTransformLocation` (`SceneComponent.K2_GetComponentToWorld` OtherComp) HitLocation) (`KismetMathLibrary.Conv_VectorToRotator` HitNormal) "KeepRelativeOffset" 30.0))
            (`DecalComponent.SetFadeScreenSize` _returnvalue_3 0.001))
          (:`Is Not Valid`
            _)))
      (`GameplayStatics.SpawnEmitterAtLocation` "/Game/kosm_fps_assets/Misc/Particles/P_IceBurst.P_IceBurst" (`self.K2_GetActorLocation`) (struct) (8.0 8.0 8.0) :!label _label)
      (`GameplayStatics.ApplyRadialDamage` :`BaseDamage` 100.0 :`Origin` _returnvalue_2 :`DamageRadius` 800.0 :`DamageCauser` self :`InstigatedByController` (`self.GetInstigatorController`))
      (`|ExecutionSequence`
        (:`then_0`
          (`ActorComponent.K2_DestroyComponent` (`self.RadialForce`))
          (`SceneComponent.SetHiddenInGame` (`self.StaticMesh`) true false)
          (`SceneComponent.SetHiddenInGame` (`self.StaticMesh1`) true false)
          (`self.SetActorEnableCollision` false)
          (`GameplayStatics.PlaySoundAtLocation` "/Game/AUDIO/SFX_Weapons/Weap_GrenadeLauncher/SC_Explosion_Flare.SC_Explosion_Flare" _returnvalue_2 (struct) 0.15 1.0 0.0 null null null)
          (`GameplayStatics.PlaySoundAtLocation` "/Game/AUDIO/SFX_Weapons/Weap_Icegun/SC_IceCrack.SC_IceCrack" _returnvalue_2 (struct) 1.5 1.0 0.0 null null null)
          (`GameplayStatics.PlayWorldCameraShake` "/Game/Blueprints/SHAKES/BP_CameraShake_Jump_Heavy.BP_CameraShake_Jump_Heavy_C" _returnvalue_2 900.0 2000.0 0.5)
          (`|SpawnActorFromClass` "/Game/Blueprints/PROJECTILES/BP_HitBurst.BP_HitBurst_C" (`self.GetTransform`) "AlwaysSpawn" "OverrideRootScale" null (0.0 0.5 1.0) (`self.GetInstigator`))
          (`|SpawnActorFromClass` "/Game/Blueprints/PROJECTILES/BP_IceBurst.BP_IceBurst_C" (`self.GetTransform`) "AlwaysSpawn" "OverrideRootScale" null _returnvalue _returnvalue)
          (`KismetSystemLibrary.Delay` 0.3)
          (`/Engine/EditorBlueprintResources/StandardMacros.IsValid` _returnvalue_3
            (:`Is Valid`
              (`ActorComponent.K2_DestroyComponent` _returnvalue_3))
            (:`Is Not Valid`
              _))
          (`self.K2_DestroyActor`))
        (:`then_2`
          (`|SpawnActorFromClass` "/Game/Blueprints/PROJECTILES/BP_IceVFX.BP_IceVFX_C" (`KismetMathLibrary.MakeTransform` (`self.K2_GetActorLocation`)) "Undefined" "OverrideRootScale" null null))))))

(event `self.Sphere.OnComponentBeginOverlap`
  (params (OverlappedComponent :type "PrimitiveComponent Object Reference") (OtherActor :type "Actor Object Reference") (OtherComp :type "PrimitiveComponent Object Reference") (OtherBodyIndex :type Integer) (bFromSweep :type Boolean) (SweepResult :type "HitResult Structure (by ref)"))
  (if (!= OtherActor (`self.GetInstigator`))
    (goto _label)))

(event `self.ProjectileMovement.OnProjectileBounce`
  (params (ImpactResult :type "HitResult Structure (by ref)") (ImpactVelocity :type "Vector Structure (by ref)"))
  (`GameplayStatics.PlaySoundAtLocation` "/Game/AUDIO/SFX_Weapons/Weap_GrenadeLauncher/SC_GrenadeHit.SC_GrenadeHit" (`self.K2_GetActorLocation`) (struct) 1.0 1.0 0.0 null null null))

(fn `UserConstructionScript`)