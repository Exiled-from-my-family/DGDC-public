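; Grenade launcher projectile that launches its physics mesh with a fixed impulse and explodes on its first hit.
; It ignores its instigator while moving and starts blocking pawns shortly after spawn.
; On hit it applies radial damage, stronger and wider for head-bone hits, fires a radial impulse, plays explosion effects, adds impact and blood decals, then destroys itself.
; Velocity checks have no effect, and bounce-sound, delay and trace logic is disconnected.
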(event `self.ReceiveBeginPlay`
  ;[0.3687 0.5739 1] Begin Play / Apply Damage / Event Hit / Line Trace
  (`PrimitiveComponent.AddImpulse` (`self.StaticMesh`) (0.0 1000.0 500.0) "None" false)
  (`KismetSystemLibrary.Delay` 0.06)
  (`PrimitiveComponent.SetCollisionResponseToChannel` (`self.StaticMesh`) "ECC_Pawn" "ECR_Block"))

(event `self.ReceiveHit`
  (params (MyComp :type "PrimitiveComponent Object Reference") (Other :type "Actor Object Reference") (OtherComp :type "PrimitiveComponent Object Reference") (bSelfMoved :type Boolean) (HitLocation :type "Vector Structure") (HitNormal :type "Vector Structure") (NormalImpulse :type "Vector Structure") (Hit :type "HitResult Structure (by ref)"))
  (bind (_bblockinghit _binitialoverlap _time _distance _location _impactpoint _normal _impactnormal _physmat _hitactor _hitcomponent _hitbonename) (`GameplayStatics.BreakHitResult` Hit))
  (bind _returnvalue (`KismetMathLibrary.Conv_VectorToRotator` _normal))
  (bind _returnvalue_2 (`KismetMathLibrary.MakeTransform` (0.0 0.0 0.0) _returnvalue))
  ;[0.3687 0.5739 1] Begin Play / Apply Damage / Event Hit / Line Trace
  (if (>= (`KismetMathLibrary.VSize` (`self.GetVelocity`)) 250.0)
    _
    (else
      _))
  (if (`.bSuccess` (cast `Character` _hitactor :!pure true))
    _
    (else
      _))
  (if (== _hitbonename "head")
    (`GameplayStatics.ApplyRadialDamage` :`BaseDamage` 150.0 :`Origin` HitLocation :`DamageRadius` 1600.0 :`DamageCauser` self :`InstigatedByController` (`self.GetInstigatorController`))
    (else
      (`GameplayStatics.ApplyRadialDamage` :`BaseDamage` 75.0 :`Origin` HitLocation :`DamageRadius` 800.0 :`DamageCauser` self :`InstigatedByController` (`self.GetInstigatorController`))))
  (`RadialForceComponent.FireImpulse` (`self.RadialForce`))
  (`GameplayStatics.SpawnEmitterAtLocation` "/Game/kosm_fps_assets/Misc/Particles/P_Explosion.P_Explosion" (`self.K2_GetActorLocation`) (struct) (5.0 5.0 5.0))
  (`GameplayStatics.PlaySoundAtLocation` "/Game/AUDIO/SFX_Weapons/Weap_GrenadeLauncher/SC_Explosion.SC_Explosion" (`SceneComponent.K2_GetComponentLocation` (`self.RadialForce`)) (struct) 0.75 1.0 0.0 null null null)
  (`/Engine/EditorBlueprintResources/StandardMacros.IsValid` _hitactor
    (:`Is Valid`
      (if (not (`self.ActorHasTag` _hitactor "Projectile"))
        (bind _returnvalue_3 (`GameplayStatics.SpawnDecalAttached` "/Game/kosm_fps_assets/Misc/Materials/BulletHole001.BulletHole001" (25.0 25.0 25.0) OtherComp "None" (`KismetMathLibrary.InverseTransformLocation` (`SceneComponent.K2_GetComponentToWorld` OtherComp) HitLocation) _returnvalue "KeepRelativeOffset" 30.0 :!label _label))
        (`DecalComponent.SetFadeScreenSize` _returnvalue_3 0.001)
        (if (`.bSuccess` (cast `Character` _hitactor :!pure true))
          (bind _returnvalue_4 (`GameplayStatics.SpawnDecalAtLocation` "/Game/kosm_fps_assets/Misc/Materials/D_BloodStain.D_BloodStain" (`KismetMathLibrary.MakeVector` (`KismetMathLibrary.RandomFloatInRange` 5.0 30.0) (`KismetMathLibrary.RandomFloatInRange` 5.0 30.0) (`KismetMathLibrary.RandomFloatInRange` 5.0 30.0)) _location (`KismetMathLibrary.MakeRotator` (`KismetMathLibrary.RandomFloatInRange` (.roll (.rotation _returnvalue_2)) 360.0) (.pitch (.rotation _returnvalue_2)) (.yaw (.rotation _returnvalue_2)))))
          (`SceneComponent.K2_AttachToComponent` _returnvalue_4 OtherComp _hitbonename "KeepWorld" "KeepWorld" "KeepWorld" true)
          (`DecalComponent.SetFadeScreenSize` _returnvalue_4 0.001)
          (`GameplayStatics.SpawnEmitterAttached` "/Game/kosm_fps_assets/Misc/Particles/PS_Blood_BulletHit.PS_Blood_BulletHit" OtherComp "None" (`KismetMathLibrary.InverseTransformLocation` (`SceneComponent.K2_GetComponentToWorld` OtherComp) HitLocation) _returnvalue (0.5 0.5 0.5)))))
    (:`Is Not Valid`
      (goto _label)))
  (`self.K2_DestroyActor`))

(fn `IgnoreActorWhenMoving`
  (`PrimitiveComponent.IgnoreActorWhenMoving` (`self.StaticMesh`) (`self.GetInstigator`) true))

(fn `UserConstructionScript`
  (`self.IgnoreActorWhenMoving`))