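; Homing missile projectile, named for a robot, that chases FpsMovementCharacter actors and explodes on contact.
; From BeginPlay it re-runs FindHomingTarget every 0.1 seconds, feeding the closest qualifying character's scene component to ProjectileMovement's homing target.
; Sphere overlap with anything but the instigator triggers explosion effects, radial damage and a force impulse, then hides and shortly destroys the missile.
; Bounces only play a sound; Hit does nothing.
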(event `Lock ON`
  (bind _target (`self.FindHomingTarget`))
  (set `ProjectileMovementComponent.HomingTargetComponent` _target (`self.ProjectileMovement`)))

(event `self.ReceiveBeginPlay`
  (`self.Lock ON` :!label _label)
  (`KismetSystemLibrary.Delay` 0.1)
  (goto _label))

(event `self.ReceiveHit`
  (params (MyComp :type "PrimitiveComponent Object Reference") (Other :type "Actor Object Reference") (OtherComp :type "PrimitiveComponent Object Reference") (bSelfMoved :type Boolean) (HitLocation :type "Vector Structure") (HitNormal :type "Vector Structure") (NormalImpulse :type "Vector Structure") (Hit :type "HitResult Structure (by ref)"))
  (if (`|EnumInequality` (`SceneComponent.Mobility` OtherComp) "Movable")
    _))

(event `self.Sphere.OnComponentBeginOverlap`
  (params (OverlappedComponent :type "PrimitiveComponent Object Reference") (OtherActor :type "Actor Object Reference") (OtherComp :type "PrimitiveComponent Object Reference") (OtherBodyIndex :type Integer) (bFromSweep :type Boolean) (SweepResult :type "HitResult Structure (by ref)"))
  (bind _returnvalue (`self.K2_GetActorLocation`))
  (bind _returnvalue_2 (`self.GetInstigatorController`))
  (if (!= OtherActor (`self.GetInstigator`))
    (`GameplayStatics.SpawnEmitterAtLocation` "/Game/kosm_fps_assets/Misc/Particles/P_Explode3.P_Explode3" (`self.K2_GetActorLocation`) (struct) (4.0 4.0 4.0))
    (`GameplayStatics.ApplyRadialDamage` 65.0 _returnvalue 800.0 null (`|MakeArray` _returnvalue_2 :!type "Actor Object Reference") self _returnvalue_2)
    (`RadialForceComponent.FireImpulse` (`self.RadialForce`))
    (`ActorComponent.K2_DestroyComponent` (`self.RadialForce`))
    (`SceneComponent.SetHiddenInGame` (`self.StaticMesh`) true false)
    (`self.SetActorEnableCollision` false)
    (`GameplayStatics.PlaySoundAtLocation` "/Game/AUDIO/SFX_Weapons/Weap_GrenadeLauncher/SC_Explosion.SC_Explosion" _returnvalue (struct) 1.0 1.0 0.0 null null null)
    (`KismetSystemLibrary.Delay` 0.3)
    (`self.K2_DestroyActor`)))

(event `self.ProjectileMovement.OnProjectileBounce`
  (params (ImpactResult :type "HitResult Structure (by ref)") (ImpactVelocity :type "Vector Structure (by ref)"))
  (`GameplayStatics.PlaySoundAtLocation` "/Game/AUDIO/SFX_Weapons/Weap_GrenadeLauncher/SC_GrenadeHit.SC_GrenadeHit" (`self.K2_GetActorLocation`) (struct) 1.0 1.0 0.0 null null null))

(fn `FindHomingTarget`
  (returns (Target :type "SceneComponent Object Reference"))
  (bind _outactors (`GameplayStatics.GetAllActorsOfClass` "/Game/Blueprints/CHARACTERS/fpsMovementCharacter_light_1_vq3.fpsMovementCharacter_light_1_vq3_C"))
  (for _array_element _outactors
    (bind _returnvalue (`KismetMathLibrary.VSize` (- (+ (`self.K2_GetActorLocation` _array_element) (0.0 0.0 150.0)) (`self.K2_GetActorLocation`))))
    (if (< _returnvalue (`self.ClosestDistance`))
      (set `self.ClosestDistance` _returnvalue)
      (set `self.HomingTarget` _array_element)))
  (return (`self.GetComponentByClass` (`self.HomingTarget`) "/Script/Engine.SceneComponent")))

(fn `UserConstructionScript`)