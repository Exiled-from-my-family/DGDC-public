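; Bubblegun projectile that bursts with radial damage, impulse, effects and camera shake, then spawns BP_BubbleBurst.
; A BeginPlay timeline grows the collision sphere and squeezes the bubble mesh, which turns toward player 0 every tick.
; It bursts on a short delay, on overlap with a non-instigator, or when its bounce counter reaches the limit.
; Overlap and bounce damage spare "Red Team"-tagged actors, while timed damage passes the instigator's controller as ignored.
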(event `self.ReceiveTick`
  (params (DeltaSeconds :type "Float (single-precision)"))
  (bind _staticmesh1 (`self.StaticMesh1`))
  (`SceneComponent.K2_SetWorldRotation` _staticmesh1 (`KismetMathLibrary.MakeRotator` (.roll (`KismetMathLibrary.FindLookAtRotation` (`SceneComponent.K2_GetComponentLocation` _staticmesh1) (`self.K2_GetActorLocation` (`GameplayStatics.GetPlayerPawn` 0)))) (- (.pitch (`KismetMathLibrary.FindLookAtRotation` (`SceneComponent.K2_GetComponentLocation` _staticmesh1) (`self.K2_GetActorLocation` (`GameplayStatics.GetPlayerPawn` 0)))) 90.0) (.yaw (`KismetMathLibrary.FindLookAtRotation` (`SceneComponent.K2_GetComponentLocation` _staticmesh1) (`self.K2_GetActorLocation` (`GameplayStatics.GetPlayerPawn` 0))))) false false))

(event `self.ReceiveBeginPlay`
  (bind _returnvalue (`self.K2_GetActorLocation`))
  (bind _returnvalue_2 (`self.GetInstigatorController`))
  (bind _staticmesh1 (`self.StaticMesh1`))
  (bind _returnvalue_3 (`SceneComponent.K2_GetComponentLocation` (`self.RadialForce`)))
  (`|ExecutionSequence`
    (:`then_0`
      (bind (_direction _bubble_squeeze _collision_size) (`Timeline|Bubble start pop` :!via `PlayFromStart` :!label _label)
        (:`Update`
          (`SphereComponent.SetSphereRadius` (`self.Sphere`) (`KismetMathLibrary.Lerp` 1.0 60.0 _collision_size) true)
          (`/Engine/EditorBlueprintResources/StandardMacros.IsValid` _staticmesh1
            (:`Is Valid`
              (`SceneComponent.SetRelativeScale3D` _staticmesh1 (`KismetMathLibrary.VLerp` (0.15 0.65 0.65) (1.35 1.35 1.35) _bubble_squeeze)))
            (:`Is Not Valid`
              _))
          (`KismetSystemLibrary.Delay` 0.575) ; old value 0,55
          (`|ExecutionSequence`
            (:`then_0`
              (goto _label :!via `Stop`))
            (:`then_1`
              (`GameplayStatics.SpawnEmitterAtLocation` "/Game/kosm_fps_assets/Misc/Particles/P_BubbleBurst1.P_BubbleBurst1" _returnvalue (struct) (4.0 4.0 4.0))
              (`GameplayStatics.SpawnEmitterAtLocation` "/Game/rpgeffects/Particles/P_Status_Teleport_Burst.P_Status_Teleport_Burst" _returnvalue (struct) (2.0 2.0 2.0))
              (`GameplayStatics.ApplyRadialDamage` (`self.DMG value`) (`self.K2_GetActorLocation`) (`self.DMG radius`) null (`|MakeArray` _returnvalue_2 :!type "Actor Object Reference") self _returnvalue_2 false "ECC_WorldStatic")
              (`RadialForceComponent.FireImpulse` (`self.RadialForce`))
              (`GameplayStatics.PlaySoundAtLocation` "/Game/AUDIO/SFX_Weapons/Weap_Bubblegun/SC_Energy_Explosion.SC_Energy_Explosion" _returnvalue_3 (struct) 1.0 1.0 0.0 null null null)
              (`GameplayStatics.PlayWorldCameraShake` "/Game/Blueprints/SHAKES/BP_CameraShake_Jump_Heavy.BP_CameraShake_Jump_Heavy_C" _returnvalue_3 900.0 1000.0)
              (`|SpawnActorFromClass` "/Game/Blueprints/PROJECTILES/BP_BubbleBurst.BP_BubbleBurst_C" (`self.GetTransform`) "Undefined" "OverrideRootScale" null null)
              (`self.K2_DestroyActor`))))))
    (:`then_2`
      (bind _outactors (`GameplayStatics.GetAllActorsWithTag` "Red Team")))))

(event `self.Sphere.OnComponentBeginOverlap`
  (params (OverlappedComponent :type "PrimitiveComponent Object Reference") (OtherActor :type "Actor Object Reference") (OtherComp :type "PrimitiveComponent Object Reference") (OtherBodyIndex :type Integer) (bFromSweep :type Boolean) (SweepResult :type "HitResult Structure (by ref)"))
  (bind _returnvalue (`SceneComponent.K2_GetComponentLocation` (`self.RadialForce`)))
  (if (!= OtherActor (`self.GetInstigator`))
    (`GameplayStatics.SpawnEmitterAtLocation` "/Game/kosm_fps_assets/Misc/Particles/P_BubbleBurst1.P_BubbleBurst1" (`self.K2_GetActorLocation`) (struct) (4.0 4.0 4.0))
    (`GameplayStatics.ApplyRadialDamage` (`self.DMG value`) (`self.K2_GetActorLocation`) (`self.DMG radius`) null (stale `self.ReceiveBeginPlay` _outactors) self (`self.GetInstigatorController`))
    (`RadialForceComponent.FireImpulse` (`self.RadialForce`))
    (`GameplayStatics.PlaySoundAtLocation` "/Game/AUDIO/SFX_Weapons/Weap_Bubblegun/SC_Energy_Explosion.SC_Energy_Explosion" _returnvalue (struct) 1.0 1.0 0.0 null null null)
    (`GameplayStatics.PlayWorldCameraShake` "/Game/Blueprints/SHAKES/BP_CameraShake_Jump_Heavy.BP_CameraShake_Jump_Heavy_C" _returnvalue 900.0 1000.0)
    (`|SpawnActorFromClass` "/Game/Blueprints/PROJECTILES/BP_BubbleBurst.BP_BubbleBurst_C" (`self.GetTransform`) "Undefined" "OverrideRootScale" null null)
    (`self.K2_DestroyActor`)))

(event `self.ProjectileMovement.OnProjectileBounce`
  (params (ImpactResult :type "HitResult Structure (by ref)") (ImpactVelocity :type "Vector Structure (by ref)"))
  (bind _returnvalue (`self.K2_GetActorLocation`))
  (bind _returnvalue_2 (`SceneComponent.K2_GetComponentLocation` (`self.StaticMesh`)))
  (bind _returnvalue_3 (`SceneComponent.K2_GetComponentLocation` (`self.RadialForce`)))
  (if (== (`self.BounceNumber`) 2.0)
    (`GameplayStatics.SpawnEmitterAtLocation` "/Game/kosm_fps_assets/Misc/Particles/P_BubbleBurst1.P_BubbleBurst1" _returnvalue (struct) (4.0 4.0 4.0))
    (`GameplayStatics.ApplyRadialDamage` (`self.DMG value`) _returnvalue (`self.DMG radius`) null (stale `self.ReceiveBeginPlay` _outactors) self (`self.GetInstigatorController`))
    (`RadialForceComponent.FireImpulse` (`self.RadialForce`))
    (`GameplayStatics.PlaySoundAtLocation` "/Game/AUDIO/SFX_Weapons/Weap_Bubblegun/SC_Energy_Explosion.SC_Energy_Explosion" _returnvalue_2 (struct) 1.0 1.0 0.0 null null null)
    (`GameplayStatics.PlayWorldCameraShake` "/Game/Blueprints/SHAKES/BP_CameraShake_Jump_Heavy.BP_CameraShake_Jump_Heavy_C" _returnvalue_2 900.0 1000.0)
    (`|SpawnActorFromClass` "/Game/Blueprints/PROJECTILES/BP_BubbleBurst.BP_BubbleBurst_C" (`self.GetTransform`) "Undefined" "OverrideRootScale" null null)
    (`self.K2_DestroyActor`)
    (else
      (`GameplayStatics.PlaySoundAtLocation` "/Game/AUDIO/SFX_Weapons/Weap_Bubblegun/SC_Energy_Bounce.SC_Energy_Bounce" _returnvalue_3 (struct) 1.5 1.0 0.0 null null null)
      (set `self.BounceNumber` (+ (`self.BounceNumber`) 1.0))
      (`GameplayStatics.SpawnEmitterAtLocation` "/Game/kosm_fps_assets/Misc/Particles/P_BubbleBurst1_1.P_BubbleBurst1_1" _returnvalue_3 (struct :`Pitch` 90.0 :`Roll` 4905.0) (2.0 1.0 2.0)))))

(fn `UserConstructionScript`)