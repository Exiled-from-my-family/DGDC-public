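; Shotgun shot projectile that spawns eight pellet projectiles on the server at BeginPlay.
; A forward trace stores target distance in ShotgunRange and disables physics simulation unless it hits a portal.
; Overlap and hit share range tiers: character impacts in the nearer two add bullet/blood effects on non-movable components and destroy the projectile; farther tiers only cast.
; Radial damage, knockback, impulse and the line-trace shot call are disconnected.
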(event `Shotgun line Trace`
  (params (`Trace start` :type "Vector Structure") (`Trace end` :type "Vector Structure"))
  (bind _outhit (`KismetSystemLibrary.LineTraceSingle` `Trace start` `Trace end` "TraceTypeQuery1" false (`|MakeArray` (`self.OwningPawn`) (`self.Instigator`) :!type "Actor Object Reference") "None" true (struct :`R` 1.0 :`A` 1.0) (struct :`G` 1.0 :`A` 1.0) 2.0))
  (bind (_bblockinghit _binitialoverlap _time _distance _location _impactpoint _normal _impactnormal _physmat _hitactor _hitcomponent) (`GameplayStatics.BreakHitResult` _outhit))
  (`/Engine/EditorBlueprintResources/StandardMacros.IsValid` _hitcomponent
    (:`Is Valid`
      (if (`|EnumInequality` (`SceneComponent.Mobility` _hitcomponent) "Movable")
        (bind _returnvalue (`GameplayStatics.SpawnDecalAttached` "/Game/kosm_fps_assets/Misc/Materials/BulletHole001.BulletHole001" (8.0 8.0 8.0) _hitcomponent "None" _location (`KismetMathLibrary.Conv_VectorToRotator` _normal) "KeepRelativeOffset" 30.0))
        (`DecalComponent.SetFadeScreenSize` _returnvalue 0.001))
      (`GameplayStatics.SpawnEmitterAtLocation` "/Game/kosm_fps_assets/Misc/Particles/P_Shotgun.P_Shotgun" _location))))

(event `self.ReceiveBeginPlay`
  (bind _collisioncomponent (`self.CollisionComponent`))
  (bind _returnvalue (`SceneComponent.K2_GetComponentLocation` _collisioncomponent))
  ;[0.3687 0.5739 1] Begin Play / Apply Damage / Event Hit / Line Trace
  (`|ExecutionSequence`
    (:`then_0`
      (bind _outactors (`GameplayStatics.GetAllActorsWithTag` "Character"))
      (bind _outactors_2 (`GameplayStatics.GetAllActorsWithTag` "Projectile"))
      (`KismetArrayLibrary.Array_Append` _outactors_2 _outactors)
      (bind _outhit (`KismetSystemLibrary.LineTraceSingle` _returnvalue (+ _returnvalue (* (`KismetMathLibrary.GetForwardVector` (`SceneComponent.K2_GetComponentRotation` _collisioncomponent)) 100000.0)) "TraceTypeQuery1" false _outactors_2))
      (`|ExecutionSequence`
        (:`then_0`
          (bind (_bblockinghit _binitialoverlap _time _distance _location _impactpoint _normal _impactnormal _physmat _hitactor) (`GameplayStatics.BreakHitResult` _outhit))
          (if (not (`.bSuccess` (cast `/Game/kosm_fps_assets/Misc/Portal/PortalBP` _hitactor :!pure true)))
            (`PrimitiveComponent.SetSimulatePhysics` (`self.CollisionComponent`) false)))
        (:`then_1`
          (set `self.Shotgun range` _distance))))
    (:`then_1`
      (`KismetSystemLibrary.Delay` 0.02)
      (`PrimitiveComponent.SetUseCCD` (`self.CollisionComponent`) true "None"))
    (:`then_2`
      (for _ (range 8)
        (`/Engine/EditorBlueprintResources/ActorMacros.Switch Has Authority`
          (:`Authority`
            (`|SpawnActorFromClass` "/Game/Blueprints/PROJECTILES/BP_Proj_Shotgun_Pellets1.BP_Proj_Shotgun_Pellets1_C" (`self.GetTransform`) "Undefined" "OverrideRootScale" null null)))))))

(event `self.CollisionComponent.OnComponentBeginOverlap`
  (params (OverlappedComponent :type "PrimitiveComponent Object Reference") (OtherActor :type "Actor Object Reference") (OtherComp :type "PrimitiveComponent Object Reference") (OtherBodyIndex :type Integer) (bFromSweep :type Boolean) (SweepResult :type "HitResult Structure (by ref)"))
  (bind _shotgun_range (`self.Shotgun range`))
  ;[0.3687 0.5739 1] Begin Play / Apply Damage / Event Hit / Line Trace
  (if (!= OtherActor (`self.GetInstigator`))
    (if (<= _shotgun_range 500.0) :!label _label
      (bind _ascharacter (cast `Character` (stale `self.ReceiveHit` Other)))
      (`/Engine/EditorBlueprintResources/StandardMacros.IsValid` (stale `self.ReceiveHit` OtherComp) :!label _label_2
        (:`Is Valid`
          (if (not (`|EnumEquality` (`SceneComponent.Mobility` (stale `self.ReceiveHit` OtherComp)) "Movable"))
            (bind _returnvalue (`KismetMathLibrary.InverseTransformLocation` (`SceneComponent.K2_GetComponentToWorld` (stale `self.ReceiveHit` OtherComp)) (stale `self.ReceiveHit` HitLocation)))
            (bind (_bblockinghit _binitialoverlap _time _distance _location _impactpoint _normal _impactnormal _physmat _hitactor) (`GameplayStatics.BreakHitResult` (stale `self.ReceiveHit` Hit)))
            (bind _returnvalue_2 (`KismetMathLibrary.Conv_VectorToRotator` _normal))
            (bind _returnvalue_3 (`GameplayStatics.SpawnDecalAttached` "/Game/kosm_fps_assets/Misc/Materials/BulletHole001.BulletHole001" (7.0 7.0 7.0) (stale `self.ReceiveHit` OtherComp) "None" _returnvalue _returnvalue_2 "SnapToTargetIncludingScale" 30.0))
            (`DecalComponent.SetFadeScreenSize` _returnvalue_3 0.001)
            (if (`.bSuccess` (cast `Character` _hitactor :!pure true))
              (bind _returnvalue_4 (`KismetMathLibrary.MakeTransform` (0.0 0.0 0.0) _returnvalue_2))
              (bind _returnvalue_5 (`GameplayStatics.SpawnDecalAtLocation` "/Game/kosm_fps_assets/Misc/Materials/D_BloodStain.D_BloodStain" (`KismetMathLibrary.MakeVector` (`KismetMathLibrary.RandomFloatInRange` 5.0 30.0) (`KismetMathLibrary.RandomFloatInRange` 5.0 30.0) (`KismetMathLibrary.RandomFloatInRange` 5.0 30.0)) _location (`KismetMathLibrary.MakeRotator` (`KismetMathLibrary.RandomFloatInRange` (.roll (.rotation _returnvalue_4)) 360.0) (.pitch (.rotation _returnvalue_4)) (.yaw (.rotation _returnvalue_4)))))
              (`DecalComponent.SetFadeScreenSize` _returnvalue_5 0.001)
              (`GameplayStatics.SpawnEmitterAttached` "/Game/kosm_fps_assets/Misc/Particles/PS_Blood_BulletHit.PS_Blood_BulletHit" (stale `self.ReceiveHit` OtherComp) "None" _returnvalue _returnvalue_2 (0.5 0.5 0.5)))))
        (:`Is Not Valid`
          _))
      (`self.K2_DestroyActor`)
      (elif (<= _shotgun_range 2000.0)
        (bind _ascharacter_2 (cast `Character` (stale `self.ReceiveHit` Other)))
        (goto _label_2)
        (elif (<= _shotgun_range 4000.0)
          (bind _ascharacter_3 (cast `Character` (stale `self.ReceiveHit` Other)))
          (else
            (bind _ascharacter_4 (cast `Character` (stale `self.ReceiveHit` Other)))))))))

(event `self.ReceiveHit`
  (params (MyComp :type "PrimitiveComponent Object Reference") (Other :type "Actor Object Reference") (OtherComp :type "PrimitiveComponent Object Reference") (bSelfMoved :type Boolean) (HitLocation :type "Vector Structure") (HitNormal :type "Vector Structure") (NormalImpulse :type "Vector Structure") (Hit :type "HitResult Structure (by ref)"))
  ;[0.3687 0.5739 1] Begin Play / Apply Damage / Event Hit / Line Trace
  (`/Engine/EditorBlueprintResources/StandardMacros.DoOnce` false
    (:`Completed`
      (goto _label))))

(fn `IgnoreActorWhenMoving`
  (`PrimitiveComponent.IgnoreActorWhenMoving` (`self.CollisionComponent`) (`self.GetInstigator`) true))

(fn `UserConstructionScript`
  (`self.IgnoreActorWhenMoving`))