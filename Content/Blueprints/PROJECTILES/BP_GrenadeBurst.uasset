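; Grenade burst projectile actor: a short-lived expanding sphere that sets characters alight on contact.
; On BeginPlay it spawns a flames projectile at its location and plays a timeline that grows the sphere and fades its dynamic material's opacity, then destroys itself.
; Any ep1_character the sphere begins overlapping gets OnFire with the burst's Causer, unless tagged Ghost.
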(event `self.ReceiveBeginPlay`
  (bind _sphere (`self.Sphere`))
  (`|SpawnActorFromClass` "/Game/Blueprints/PROJECTILES/BP_Proj_Flames.BP_Proj_Flames_C" (`KismetMathLibrary.MakeTransform` (`self.K2_GetActorLocation`)) "Undefined" "OverrideRootScale" null null)
  (bind (_direction _newtrack_0) (`Timeline|Burst` :!via `PlayFromStart`)
    (:`Update`
      (`MeshComponent.SetScalarParameterValueOnMaterials` _sphere "opacity" (`KismetMathLibrary.Lerp` 0.25 0.0 _newtrack_0))
      (`SceneComponent.SetRelativeScale3D` _sphere (`KismetMathLibrary.VLerp` (2.0 2.0 2.0) (20.0 20.0 20.0) _newtrack_0)))
    (:`Finished`
      (`self.K2_DestroyActor`))))

(event `self.Sphere.OnComponentBeginOverlap`
  (params (OverlappedComponent :type "PrimitiveComponent Object Reference") (OtherActor :type "Actor Object Reference") (OtherComp :type "PrimitiveComponent Object Reference") (OtherBodyIndex :type Integer) (bFromSweep :type Boolean) (SweepResult :type "HitResult Structure (by ref)"))
  (bind _asep_1_character (cast `/Game/MISSIONS/EP1/Characters/ep1_character` OtherActor))
  (if (not (`self.ActorHasTag` _asep_1_character "Ghost"))
    (`/Game/MISSIONS/EP1/Characters/ep1_character.OnFire` _asep_1_character (`self.causer`))))

(fn `UserConstructionScript`
  (bind _sphere (`self.Sphere`))
  (`PrimitiveComponent.CreateDynamicMaterialInstance` _sphere 0 "/Game/MATERIALS/M_vegasLight_Inst4.M_vegasLight_Inst4" "None")
  (`MeshComponent.SetScalarParameterValueOnMaterials` _sphere "opacity" 1.0))