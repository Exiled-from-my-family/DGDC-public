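; Charged Sonic Gun projectile that spends sonic ammo on spawn and blasts the player up and backward when fired at a nearby surface.
; Non-static targets take radial damage, and characters not tagged Ghost, Molly or TooBig are launched with briefly lowered ground friction.
; Impacts, including static ones, spawn burst effects and stun robots and turrets in a wide radius before the projectile destroys itself.
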(event `self.ReceiveBeginPlay`
  (bind _collisioncomponent (`self.CollisionComponent`))
  (bind _returnvalue (`SceneComponent.K2_GetComponentLocation` _collisioncomponent))
  (`/Engine/EditorBlueprintResources/ActorMacros.Switch Has Authority`
    (:`Authority`
      (set `self.StartLocation` (`SceneComponent.K2_GetComponentLocation` (`self.CollisionComponent`)))
      (bind _player (`/Game/Blueprints/NewFunctionLibrary.get player`))
      (set `/Game/Blueprints/CHARACTERS/fpsMovementCharacter_light_1_vq3.SonicCharged?` false _player)
      (set `/Game/Blueprints/CHARACTERS/fpsMovementCharacter_light_1_vq3.SonicAmmo` (- (`/Game/Blueprints/CHARACTERS/fpsMovementCharacter_light_1_vq3.SonicAmmo` _player) 4) _player)
      (bind (_outhit _returnvalue_2) (`KismetSystemLibrary.SphereTraceSingle` _returnvalue (+ _returnvalue (* (`KismetMathLibrary.GetForwardVector` (`SceneComponent.K2_GetComponentRotation` _collisioncomponent)) 500.0)) 10.0 "TraceTypeQuery1"))
      (if _returnvalue_2
        (bind _player_2 (`/Game/Blueprints/NewFunctionLibrary.get player`))
        (`Character.LaunchCharacter` _player_2 (0.0 0.0 900.0) false false)
        (`KismetSystemLibrary.Delay` 0.1)
        (`Character.LaunchCharacter` _player_2 (* (`KismetMathLibrary.GetForwardVector` (`PlayerCameraManager.GetCameraRotation` (`GameplayStatics.GetPlayerCameraManager` 0))) -1850.0) false false)))
    (:`Remote`
      (`self.K2_DestroyActor`))))

(event `self.CollisionComponent.OnComponentBeginOverlap`
  (params (OverlappedComponent :type "PrimitiveComponent Object Reference") (OtherActor :type "Actor Object Reference") (OtherComp :type "PrimitiveComponent Object Reference") (OtherBodyIndex :type Integer) (bFromSweep :type Boolean) (SweepResult :type "HitResult Structure (by ref)"))
  (if (!= OtherActor (`self.GetInstigator`))
    (if (or (`self.ActorHasTag` (stale `self.ReceiveHit` Other) "Ghost") (`self.ActorHasTag` (stale `self.ReceiveHit` Other) "Molly") (`self.ActorHasTag` (stale `self.ReceiveHit` Other) "TooBig")) :!label _label
      (`KismetSystemLibrary.PrintString` "NO BOOP" true false)
      (`GameplayStatics.ApplyRadialDamage` :`BaseDamage` 60.0 :`Origin` (`self.K2_GetActorLocation`) :`DamageRadius` 750.0 :`DamageCauser` self :`InstigatedByController` (`self.GetInstigatorController`) :`DamagePreventionChannel` "ECC_GameTraceChannel2")
      (else
        (`GameplayStatics.ApplyRadialDamage` :`BaseDamage` 60.0 :`Origin` (`self.K2_GetActorLocation`) :`DamageRadius` 750.0 :`DamageCauser` self :`InstigatedByController` (`self.GetInstigatorController`) :`DamagePreventionChannel` "ECC_GameTraceChannel2")
        (bind _ascharacter (cast `Character` (stale `self.ReceiveHit` Other)))
        (bind _charactermovement (`Character.CharacterMovement` _ascharacter))
        (set `CharacterMovementComponent.GroundFriction` 0.2 _charactermovement)
        (`Character.LaunchCharacter` _ascharacter (0.0 0.0 1200.0) false false)
        (`KismetSystemLibrary.Delay` 0.05)
        (`Character.LaunchCharacter` _ascharacter (* (`SceneComponent.GetForwardVector` (`self.CollisionComponent`)) 2400.0) true false)
        (set `CharacterMovementComponent.GroundFriction` 6.0 _charactermovement)))
    (`GameplayStatics.SpawnEmitterAtLocation` "/Game/kosm_fps_assets/Misc/Particles/P_IceBurst1.P_IceBurst1" (`self.K2_GetActorLocation`) (struct) (2.0 2.0 2.0) :!label _label_2)
    (`|SpawnActorFromClass` "/Game/Blueprints/PROJECTILES/BP_HitBurst.BP_HitBurst_C" (`KismetMathLibrary.MakeTransform` (stale `self.ReceiveHit` HitLocation) (struct) (0.7 0.7 0.7)) "Undefined" "OverrideRootScale" null (0.0 0.25 0.75) null)
    (`|ExecutionSequence`
      (:`then_0`
        (`/Game/MISSIONS/EP1/BP_MyMacroLibrary.For Loop With Delay` 0 2 0.075
          (:`Loop Body`
            (`|SpawnActorFromClass` "/Game/Blueprints/PROJECTILES/BP_SonicBurst.BP_SonicBurst_C" (`KismetMathLibrary.MakeTransform` (stale `self.ReceiveHit` HitLocation)) "Undefined" "OverrideRootScale" null null))))
      (:`then_1`
        (bind _outhits (`KismetSystemLibrary.SphereTraceMultiForObjects` (stale `self.ReceiveHit` HitLocation) (stale `self.ReceiveHit` HitLocation) 1000.0 (`|MakeArray` "ObjectTypeQuery3" :!type "EObjectTypeQuery Enum")))
        (for _array_element _outhits
          (bind (_bblockinghit _binitialoverlap _time _distance _location _impactpoint _normal _impactnormal _physmat _hitactor) (`GameplayStatics.BreakHitResult` _array_element))
          (bind (_asep3_robot _bsuccess) (cast `/Game/MISSIONS/EP3/Characters/EP3_robot` _hitactor :!pure true))
          (if _bsuccess
            (`/Game/MISSIONS/EP3/Characters/EP3_robot.Stunned` _asep3_robot)
            (else
              (bind (_asep3_robot_mid _bsuccess_2) (cast `/Game/MISSIONS/EP3/Characters/EP3_robot_mid` _hitactor :!pure true))
              (if _bsuccess_2
                (`/Game/MISSIONS/EP3/Characters/EP3_robot_mid.Stunned` _asep3_robot_mid)
                (else
                  (bind (_asep6_turret _bsuccess_3) (cast `/Game/MISSIONS/EP6/Characters/EP6_Turret` _hitactor :!pure true))
                  (if _bsuccess_3
                    (`/Game/MISSIONS/EP6/Characters/EP6_Turret.Stunned` _asep6_turret)))))))
        (`KismetSystemLibrary.Delay` 1.0)
        (`self.K2_DestroyActor`)))))

(event `self.ReceiveHit`
  (params (MyComp :type "PrimitiveComponent Object Reference") (Other :type "Actor Object Reference") (OtherComp :type "PrimitiveComponent Object Reference") (bSelfMoved :type Boolean) (HitLocation :type "Vector Structure") (HitNormal :type "Vector Structure") (NormalImpulse :type "Vector Structure") (Hit :type "HitResult Structure (by ref)"))
  (if (!= Other (`self.GetInstigator`))
    (if (`|EnumInequality` (`SceneComponent.Mobility` OtherComp) "Static")
      (goto _label)
      (else
        (goto _label_2)))))

(fn `IgnoreActorWhenMoving`
  (`PrimitiveComponent.IgnoreActorWhenMoving` (`self.CollisionComponent`) (`self.GetInstigator`) true))

(fn `UserConstructionScript`
  (`self.IgnoreActorWhenMoving`))