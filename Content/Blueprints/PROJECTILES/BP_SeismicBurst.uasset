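; Seismic burst shockwave actor that shakes the camera, plays a hammer-break sound and knocks a character airborne on spawn.
; A ring of horizontal box traces, ignoring Ep2_blue_hacker_takes_over_rumble actors, finds player-class characters; a DoOnce launches and stuns only the first hit.
; A timeline expands and fades the sphere visual, then the actor destroys itself after a delay.
; Damage nodes are unwired, and the overlap event only prints a debug string.
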(event `self.ReceiveBeginPlay`
  (bind _returnvalue (`self.K2_GetActorLocation`))
  (bind _returnvalue_2 (`self.K2_GetActorLocation`))
  (bind _sphere (`self.Sphere`))
  (bind _newvar_0 (`self.NewVar_0`))
  (`GameplayStatics.PlayWorldCameraShake` "/Game/Blueprints/SHAKES/BP_CameraShake_Explosion.BP_CameraShake_Explosion_C" _returnvalue_2 1800.0 3000.0 0.2)
  (`|ExecutionSequence`
    (:`then_0`
      (bind _outactors (`GameplayStatics.GetAllActorsOfClass` "/Game/MISSIONS/EP2/Characters/ep2_blue_hacker_takes_over_rumble.ep2_blue_hacker_takes_over_rumble_C"))
      (for _index (range (+ _newvar_0 1))
        (bind (_outhit _returnvalue_3) (`KismetSystemLibrary.BoxTraceSingle` _returnvalue (+ _returnvalue (* (`KismetMathLibrary.GreaterGreater_VectorRotator` (`self.GetActorForwardVector`) (`KismetMathLibrary.MakeRotator` 0.0 0.0 (* _index (/ 360.0 (`KismetMathLibrary.Conv_IntToDouble` (+ _newvar_0 1)))))) 1800.0)) (8.0 8.0 36.0) (struct) "TraceTypeQuery1" false _outactors "None" true (struct :`R` 1.0 :`A` 1.0) (struct :`G` 1.0 :`A` 1.0) 2.0))
        (if _returnvalue_3
          (bind _asfps_movement_character_light_1_vq_3 (cast `/Game/Blueprints/CHARACTERS/fpsMovementCharacter_light_1_vq3` (`.HitActor` (`GameplayStatics.BreakHitResult` _outhit))))
          (`/Engine/EditorBlueprintResources/StandardMacros.DoOnce` false
            (:`Completed`
              (`Character.LaunchCharacter` _asfps_movement_character_light_1_vq_3 (`KismetMathLibrary.MakeVector` (`KismetMathLibrary.RandomFloatInRange` -800.0 800.0) (`KismetMathLibrary.RandomFloatInRange` -800.0 800.0) 4000.0) false false)
              (`/Game/Blueprints/CHARACTERS/fpsMovementCharacter_light_1_vq3.Stunned_InAir` _asfps_movement_character_light_1_vq_3 0.9))))))
    (:`then_1`
      (bind (_direction _newtrack_0) (`Timeline|Burst` :!via `PlayFromStart`)
        (:`Update`
          (`MeshComponent.SetScalarParameterValueOnMaterials` _sphere "opacity" (`KismetMathLibrary.Lerp` 0.6 0.0 _newtrack_0))
          (`SceneComponent.SetRelativeScale3D` _sphere (`KismetMathLibrary.VLerp` (2.0 2.0 2.0) (34.0 34.0 12.0) _newtrack_0)))
        (:`Finished`
          (`KismetSystemLibrary.Delay` 2.0)
          (`self.K2_DestroyActor`))))
    (:`then_2`
      (`GameplayStatics.SpawnSoundAtLocation` "/Game/AUDIO/SFX_Weapons/Weap_Hammer/SW_HammerBreak.SW_HammerBreak" _returnvalue_2 (struct) 1.0 1.0 0.0 "/Game/kosm_fps_assets/Misc/SoundFX/SoundAttenuationNormal.SoundAttenuationNormal" null))))

(event `self.Sphere1.OnComponentBeginOverlap`
  (params (OverlappedComponent :type "PrimitiveComponent Object Reference") (OtherActor :type "Actor Object Reference") (OtherComp :type "PrimitiveComponent Object Reference") (OtherBodyIndex :type Integer) (bFromSweep :type Boolean) (SweepResult :type "HitResult Structure (by ref)"))
  (bind _asfps_movement_character_light_1_vq_3 (cast `/Game/Blueprints/CHARACTERS/fpsMovementCharacter_light_1_vq3` OtherActor))
  (`KismetSystemLibrary.PrintString` "Hello"))

(fn `UserConstructionScript`
  (bind _sphere (`self.Sphere`))
  (`PrimitiveComponent.CreateDynamicMaterialInstance` _sphere 0 "/Game/MATERIALS/M_vegasLight_Inst1.M_vegasLight_Inst1" "None")
  (`MeshComponent.SetScalarParameterValueOnMaterials` _sphere "opacity" 1.0))