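; Shotgun blast projectile that spawns twelve pellet actors on the server and knocks Characters back by range.
; BeginPlay traces forward to store ShotgunRange, while a timeline widens the collision sphere.
; Overlap or first hit (which also fires a radial impulse) picks a range band for two-step launches, with camera shake, blood or decals, and destruction only in the two nearest.
; Radial damage and the pellet line-trace call are disconnected.
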(event `Shotgun line Trace`
  (params (`Trace start` :type "Vector Structure") (`Trace end` :type "Vector Structure"))
  (bind _outhit (`KismetSystemLibrary.LineTraceSingle` `Trace start` `Trace end` "TraceTypeQuery1" false (`|MakeArray` (`self.OwningPawn`) (`self.Instigator`) :!type "Actor Object Reference") "None" true (struct :`R` 1.0 :`A` 1.0) (struct :`G` 1.0 :`A` 1.0) 2.0))
  (bind (_bblockinghit _binitialoverlap _time _distance _location _impactpoint _normal _impactnormal _physmat _hitactor _hitcomponent) (`GameplayStatics.BreakHitResult` _outhit))
  (`/Engine/EditorBlueprintResources/StandardMacros.IsValid` _hitcomponent
    (:`Is Valid`
      (`GameplayStatics.SpawnEmitterAtLocation` "/Game/kosm_fps_assets/Misc/Particles/P_NailgunImpact.P_NailgunImpact" _location (struct) (0.5 0.5 0.5)))))

(event `self.ReceiveBeginPlay`
  (bind _collisioncomponent (`self.CollisionComponent`))
  (bind _returnvalue (`SceneComponent.K2_GetComponentLocation` _collisioncomponent))
  ;[0.3687 0.5739 1] Begin Play / Apply Damage / Event Hit / Line Trace
  (`|ExecutionSequence`
    (:`then_0`
      (bind _outactors (`GameplayStatics.GetAllActorsWithTag` "Character"))
      (bind _outactors_2 (`GameplayStatics.GetAllActorsWithTag` "Projectile"))
      (`KismetArrayLibrary.Array_Append` _outactors_2 _outactors)
      (bind _outhit (`KismetSystemLibrary.LineTraceSingle` _returnvalue (+ _returnvalue (* (`KismetMathLibrary.GetForwardVector` (`SceneComponent.K2_GetComponentRotation` _collisioncomponent)) 100000.0)) "TraceTypeQuery1" false _outactors_2))
      (`|ExecutionSequence`
        (:`then_0`
          (bind (_direction _newtrack_0) (`Timeline|Timeline_0` :!via `PlayFromStart`)
            (:`Update`
              (`SphereComponent.SetSphereRadius` (`self.CollisionComponent`) (`KismetMathLibrary.Lerp` 40.0 200.0 _newtrack_0) true)
              (bind (_bblockinghit _binitialoverlap _time _distance _location _impactpoint _normal _impactnormal _physmat _hitactor) (`GameplayStatics.BreakHitResult` _outhit))
              (if (not (`.bSuccess` (cast `/Game/kosm_fps_assets/Misc/Portal/PortalBP` _hitactor :!pure true)))
                (`PrimitiveComponent.SetSimulatePhysics` (`self.CollisionComponent`) false)))))
        (:`then_1`
          (set `self.Shotgun range` _distance))))
    (:`then_1`
      (`KismetSystemLibrary.Delay` 0.02)
      (`PrimitiveComponent.SetUseCCD` (`self.CollisionComponent`) true "None"))
    (:`then_2`
      (for _ (range 12)
        (`/Engine/EditorBlueprintResources/ActorMacros.Switch Has Authority`
          (:`Authority`
            (`|SpawnActorFromClass` "/Game/Blueprints/PROJECTILES/BP_Proj_Shotgun_Pellets.BP_Proj_Shotgun_Pellets_C" (`self.GetTransform`) "Undefined" "OverrideRootScale" null null)))))))

(event `self.CollisionComponent.OnComponentBeginOverlap`
  (params (OverlappedComponent :type "PrimitiveComponent Object Reference") (OtherActor :type "Actor Object Reference") (OtherComp :type "PrimitiveComponent Object Reference") (OtherBodyIndex :type Integer) (bFromSweep :type Boolean) (SweepResult :type "HitResult Structure (by ref)"))
  (bind _shotgun_range (`self.Shotgun range`))
  (bind _returnvalue (`SceneComponent.GetForwardVector` (`self.CollisionComponent`)))
  ;[0.3687 0.5739 1] Begin Play / Apply Damage / Event Hit / Line Trace
  (if (!= OtherActor (`self.GetInstigator`))
    (bind _outactors (`GameplayStatics.GetAllActorsWithTag` "Red Team" :!label _label))
    (if (<= _shotgun_range 400.0)
      (`PlayerCameraManager.PlayCameraShake` :`self` (`GameplayStatics.GetPlayerCameraManager` 0) :`ShakeClass` "/Game/Blueprints/SHAKES/BP_CameraShake_Jump_Heavy.BP_CameraShake_Jump_Heavy_C" :`Scale` 2.0)
      (bind _ascharacter (cast `Character` (stale `self.ReceiveHit` Other)))
      (`Character.LaunchCharacter` _ascharacter (0.0 0.0 900.0) false false)
      (`KismetSystemLibrary.Delay` 0.1)
      (`Character.LaunchCharacter` _ascharacter (* _returnvalue 3700.0) false false)
      (`/Engine/EditorBlueprintResources/StandardMacros.IsValid` (stale `self.ReceiveHit` OtherComp) :!label _label_2
        (:`Is Valid`
          (if (`|EnumEquality` (`SceneComponent.Mobility` (stale `self.ReceiveHit` OtherComp)) "Movable")
            (bind (_bblockinghit _binitialoverlap _time _distance _location _impactpoint _normal _impactnormal _physmat _hitactor) (`GameplayStatics.BreakHitResult` (stale `self.ReceiveHit` Hit)))
            (if (`self.ActorHasTag` _hitactor "Undead")
              (bind (_outhit _returnvalue_2) (`KismetSystemLibrary.LineTraceSingle` (stale `self.ReceiveHit` HitLocation) (+ (stale `self.ReceiveHit` HitLocation) (* (`KismetMathLibrary.GetUpVector` (`KismetMathLibrary.FindLookAtRotation` (`self.K2_GetActorLocation`) (stale `self.ReceiveHit` HitLocation))) -300.0)) "TraceTypeQuery1"))
              (if _returnvalue_2
                (bind (_bblockinghit_2 _binitialoverlap_2 _time_2 _distance_2 _location_2 _impactpoint_2 _normal_2) (`GameplayStatics.BreakHitResult` _outhit))
                (bind _returnvalue_3 (`GameplayStatics.SpawnDecalAtLocation` (select `int` (`KismetMathLibrary.RandomIntegerInRange` 0 7) :`0` "/Game/kosm_fps_assets/Misc/Materials/D_BloodStain_Inst.D_BloodStain_Inst" :`1` "/Game/kosm_fps_assets/Misc/Materials/D_BloodStain_Inst1.D_BloodStain_Inst1" :`2` "/Game/kosm_fps_assets/Misc/Materials/D_BloodStain_Inst2.D_BloodStain_Inst2" :`3` "/Game/kosm_fps_assets/Misc/Materials/D_BloodStain_Inst3.D_BloodStain_Inst3" :`4` "/Game/kosm_fps_assets/Misc/Materials/D_BloodStain_Inst4.D_BloodStain_Inst4" :`5` "/Game/kosm_fps_assets/Misc/Materials/D_BloodStain_Inst5.D_BloodStain_Inst5" :`6` "/Game/kosm_fps_assets/Misc/Materials/D_BloodStain_Inst6.D_BloodStain_Inst6" :`7` "/Game/kosm_fps_assets/Misc/Materials/D_BloodStain_Inst7.D_BloodStain_Inst7" :!type "MaterialInterface Object Reference") (`KismetMathLibrary.MakeVector` (`KismetMathLibrary.RandomFloatInRange` 100.0 120.0) (`KismetMathLibrary.RandomFloatInRange` 100.0 120.0) (`KismetMathLibrary.RandomFloatInRange` 100.0 120.0)) _location_2 (`KismetMathLibrary.MakeRotFromX` _normal_2) 10.0))
                (`DecalComponent.SetFadeScreenSize` _returnvalue_3 0.001))
              (`GameplayStatics.SpawnEmitterAttached` "/Game/kosm_fps_assets/Misc/Particles/PS_Blood_BulletHit1.PS_Blood_BulletHit1" null "None" (0.0 0.0 0.0) (struct) (0.75 0.75 0.75)))
            (else
              (bind _returnvalue_4 (`GameplayStatics.SpawnDecalAttached` null (7.0 7.0 7.0) (stale `self.ReceiveHit` OtherComp) "None" (`KismetMathLibrary.InverseTransformLocation` (`SceneComponent.K2_GetComponentToWorld` (stale `self.ReceiveHit` OtherComp)) (stale `self.ReceiveHit` HitLocation)) (`KismetMathLibrary.Conv_VectorToRotator` _normal) "SnapToTargetIncludingScale" 30.0))
              (`DecalComponent.SetFadeScreenSize` _returnvalue_4 0.001))))
        (:`Is Not Valid`
          _))
      (`self.K2_DestroyActor`)
      (elif (<= _shotgun_range 2000.0)
        (`PlayerCameraManager.PlayCameraShake` :`self` (`GameplayStatics.GetPlayerCameraManager` 0) :`ShakeClass` "/Game/Blueprints/SHAKES/BP_CameraShake_Jump_Heavy.BP_CameraShake_Jump_Heavy_C")
        (bind _ascharacter_2 (cast `Character` (stale `self.ReceiveHit` Other)))
        (`Character.LaunchCharacter` _ascharacter_2 (0.0 0.0 700.0) false false)
        (`KismetSystemLibrary.Delay` 0.1)
        (`Character.LaunchCharacter` _ascharacter_2 (* _returnvalue 3000.0) false false)
        (goto _label_2)
        (elif (<= _shotgun_range 4000.0)
          (bind _ascharacter_3 (cast `Character` (stale `self.ReceiveHit` Other)))
          (`Character.LaunchCharacter` _ascharacter_3 (0.0 0.0 300.0) false false)
          (`KismetSystemLibrary.Delay` 0.1)
          (`Character.LaunchCharacter` _ascharacter_3 (* _returnvalue 3000.0) false false)
          (else
            (bind _ascharacter_4 (cast `Character` (stale `self.ReceiveHit` Other)))
            (`Character.LaunchCharacter` _ascharacter_4 (0.0 0.0 50.0) false false)
            (`KismetSystemLibrary.Delay` 0.1)
            (`Character.LaunchCharacter` _ascharacter_4 (* _returnvalue 1200.0) false false)))))))

(event `self.ReceiveHit`
  (params (MyComp :type "PrimitiveComponent Object Reference") (Other :type "Actor Object Reference") (OtherComp :type "PrimitiveComponent Object Reference") (bSelfMoved :type Boolean) (HitLocation :type "Vector Structure") (HitNormal :type "Vector Structure") (NormalImpulse :type "Vector Structure") (Hit :type "HitResult Structure (by ref)"))
  ;[0.3687 0.5739 1] Begin Play / Apply Damage / Event Hit / Line Trace
  (`/Engine/EditorBlueprintResources/StandardMacros.DoOnce` false
    (:`Completed`
      (`RadialForceComponent.FireImpulse` (`self.RadialForce`))
      (goto _label))))

(fn `IgnoreActorWhenMoving`
  (`PrimitiveComponent.IgnoreActorWhenMoving` (`self.CollisionComponent`) (`self.GetInstigator`) true))

(fn `UserConstructionScript`
  (`self.IgnoreActorWhenMoving`))