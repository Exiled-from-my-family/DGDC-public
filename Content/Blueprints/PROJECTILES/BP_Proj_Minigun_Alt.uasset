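; Minigun alt-fire bullet that launches at extreme speed with random spread, ignoring its instigator.
; BeginPlay draws a beam from the shooter's first-person muzzle to a separately randomized endpoint; its line trace result is unused.
; Hits on movable components apply small radial damage sparing "Red Team", with blood particles and traced blood decals for "Undead" characters.
; Other surfaces get impact particles, ricochet sound and bullet-hole decals; the actor is destroyed after a short delay.
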(event `CustomEvent_0`
  (params (Start :type "Vector Structure") (End :type "Vector Structure"))
  (`ParticleSystemComponent.SetBeamSourcePoint` (`self.ParticleSystem`) 0 (`SceneComponent.K2_GetComponentLocation` (`/Game/Blueprints/CHARACTERS/fpsMovementCharacter_light_1_vq3.Muzzle1P` (cast `/Game/Blueprints/CHARACTERS/fpsMovementCharacter_light_1_vq3` (`self.GetInstigator`) :!pure true))) 0)
  (`ParticleSystemComponent.SetBeamEndPoint` (`self.ParticleSystem`) 0 End))

(event `self.ReceiveBeginPlay`
  (bind _spread (`self.Spread`))
  (bind _returnvalue (`SceneComponent.K2_GetComponentLocation` (`self.CollisionComponent`)))
  (bind _returnvalue_2 (* _spread -1.0))
  (bind _returnvalue_3 (`KismetMathLibrary.RandomFloatInRange` _returnvalue_2 _spread))
  (bind _returnvalue_4 (`KismetMathLibrary.RandomFloatInRange` _returnvalue_2 _spread))
  (bind _returnvalue_5 (+ (+ _returnvalue (* (`SceneComponent.GetForwardVector` (`self.CollisionComponent`)) 8000.0)) (`KismetMathLibrary.MakeVector` _returnvalue_4 _returnvalue_3 (`KismetMathLibrary.RandomFloatInRange` _returnvalue_2 _spread))))
  (`ProjectileMovementComponent.SetVelocityInLocalSpace` (`self.Projectile`) (`KismetMathLibrary.MakeVector` 100000000.0 _returnvalue_4 _returnvalue_3))
  (set `ProjectileMovementComponent.bRotationFollowsVelocity` true (`self.Projectile`))
  (`self.CustomEvent_0` _returnvalue _returnvalue_5)
  (`KismetSystemLibrary.LineTraceSingle` _returnvalue _returnvalue_5 "TraceTypeQuery1" false (`|MakeArray` (`self.NewVar_0`) (`self.Instigator`) :!type "Actor Object Reference") "None" true (struct :`R` 1.0 :`A` 1.0) (struct :`G` 1.0 :`A` 1.0) 2.0))

(event `self.CollisionComponent.OnComponentHit`
  (params (HitComponent :type "PrimitiveComponent Object Reference") (OtherActor :type "Actor Object Reference") (OtherComp :type "PrimitiveComponent Object Reference") (NormalImpulse :type "Vector Structure") (Hit :type "HitResult Structure (by ref)"))
  (bind (_bblockinghit _binitialoverlap _time _distance _location _impactpoint _normal _impactnormal _physmat _hitactor _hitcomponent _hitbonename) (`GameplayStatics.BreakHitResult` Hit))
  (bind _returnvalue (`KismetMathLibrary.Conv_VectorToRotator` _normal))
  ;[0.3687 0.5739 1] Begin Play / Apply Damage / Event Hit / Line Trace
  (bind _outactors (`GameplayStatics.GetAllActorsWithTag` "Red Team"))
  (if (`|EnumEquality` (`SceneComponent.Mobility` _hitcomponent) "Movable")
    (`GameplayStatics.ApplyRadialDamage` 11.0 _location 10.0 null _outactors self (`self.GetInstigatorController`) true)
    (if (and (`self.ActorHasTag` _hitactor "Undead") (`.bSuccess` (cast `Character` _hitactor :!pure true)))
      (bind (_outhit _returnvalue_2) (`KismetSystemLibrary.LineTraceSingle` _location (+ _location (* (`KismetMathLibrary.GetUpVector` (`KismetMathLibrary.FindLookAtRotation` (`self.K2_GetActorLocation`) _location)) -300.0)) "TraceTypeQuery1"))
      (if _returnvalue_2
        (bind (_bblockinghit_2 _binitialoverlap_2 _time_2 _distance_2 _location_2 _impactpoint_2 _normal_2) (`GameplayStatics.BreakHitResult` _outhit))
        (bind _returnvalue_3 (`GameplayStatics.SpawnDecalAtLocation` (select `int` (`KismetMathLibrary.RandomIntegerInRange` 0 7) :`0` "/Game/kosm_fps_assets/Misc/Materials/D_BloodStain_Inst.D_BloodStain_Inst" :`1` "/Game/kosm_fps_assets/Misc/Materials/D_BloodStain_Inst1.D_BloodStain_Inst1" :`2` "/Game/kosm_fps_assets/Misc/Materials/D_BloodStain_Inst2.D_BloodStain_Inst2" :`3` "/Game/kosm_fps_assets/Misc/Materials/D_BloodStain_Inst3.D_BloodStain_Inst3" :`4` "/Game/kosm_fps_assets/Misc/Materials/D_BloodStain_Inst4.D_BloodStain_Inst4" :`5` "/Game/kosm_fps_assets/Misc/Materials/D_BloodStain_Inst5.D_BloodStain_Inst5" :`6` "/Game/kosm_fps_assets/Misc/Materials/D_BloodStain_Inst6.D_BloodStain_Inst6" :`7` "/Game/kosm_fps_assets/Misc/Materials/D_BloodStain_Inst7.D_BloodStain_Inst7" :!type "MaterialInterface Object Reference") (`KismetMathLibrary.MakeVector` (`KismetMathLibrary.RandomFloatInRange` 100.0 120.0) (`KismetMathLibrary.RandomFloatInRange` 100.0 120.0) (`KismetMathLibrary.RandomFloatInRange` 100.0 120.0)) _location_2 (`KismetMathLibrary.MakeRotFromX` _normal_2) 10.0))
        (`DecalComponent.SetFadeScreenSize` _returnvalue_3 0.001))
      (`GameplayStatics.SpawnEmitterAtLocation` "/Game/kosm_fps_assets/Misc/Particles/PS_Blood_BulletHit1.PS_Blood_BulletHit1" _location _returnvalue))
    (else
      (`GameplayStatics.SpawnEmitterAtLocation` "/Game/kosm_fps_assets/Misc/Particles/P_MinigunImpact.P_MinigunImpact" _location (struct) (0.75 0.75 0.75))
      (`GameplayStatics.PlaySoundAtLocation` "/Game/AUDIO/SFX_Weapons/Weap_Minigun/SC_Minigun_Ricochet.SC_Minigun_Ricochet" _location (struct) 1.0 1.0 0.0 null null null)
      (bind _returnvalue_4 (`GameplayStatics.SpawnDecalAttached` "/Game/kosm_fps_assets/Misc/Materials/BulletHole001.BulletHole001" (4.0 4.0 4.0) _hitcomponent "None" (`KismetMathLibrary.InverseTransformLocation` (`SceneComponent.K2_GetComponentToWorld` _hitcomponent) _location) _returnvalue "KeepRelativeOffset" 30.0))
      (`DecalComponent.SetFadeScreenSize` _returnvalue_4 0.001)))
  (`KismetSystemLibrary.Delay` 2.0)
  (`self.K2_DestroyActor`))

(event `self.StaticMesh.OnComponentHit`
  (params (HitComponent :type "PrimitiveComponent Object Reference") (OtherActor :type "Actor Object Reference") (OtherComp :type "PrimitiveComponent Object Reference") (NormalImpulse :type "Vector Structure") (Hit :type "HitResult Structure (by ref)"))
  (`ActorComponent.K2_DestroyComponent` (`self.StaticMesh`)))

(fn `IgnoreActorWhenMoving`
  (`PrimitiveComponent.IgnoreActorWhenMoving` (`self.CollisionComponent`) (`self.GetInstigator`) true))

(fn `UserConstructionScript`
  (`self.IgnoreActorWhenMoving`))