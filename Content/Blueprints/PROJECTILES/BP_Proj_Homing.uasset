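; Bouncing bubble projectile that homes in on a living ep1_character and bursts with radial damage, sparing actors tagged "Red Team".
; Overlapping the Sphere1 trigger switches ProjectileMovement to homing once, while the mesh turns toward the player every tick.
; Hits, non-instigator overlaps or reaching the bounce limit trigger impulse, effects, camera shake and a BP_BubbleBurst spawn.
; The pop-in timeline, trace timer and delayed detonations are disconnected.
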(event `self.ReceiveTick`
  (params (DeltaSeconds :type "Float (single-precision)"))
  (bind _staticmesh1 (`self.StaticMesh1`))
  (`SceneComponent.K2_SetWorldRotation` _staticmesh1 (`KismetMathLibrary.MakeRotator` (.roll (`KismetMathLibrary.FindLookAtRotation` (`SceneComponent.K2_GetComponentLocation` _staticmesh1) (`self.K2_GetActorLocation` (`GameplayStatics.GetPlayerPawn` 0)))) (- (.pitch (`KismetMathLibrary.FindLookAtRotation` (`SceneComponent.K2_GetComponentLocation` _staticmesh1) (`self.K2_GetActorLocation` (`GameplayStatics.GetPlayerPawn` 0)))) 90.0) (.yaw (`KismetMathLibrary.FindLookAtRotation` (`SceneComponent.K2_GetComponentLocation` _staticmesh1) (`self.K2_GetActorLocation` (`GameplayStatics.GetPlayerPawn` 0))))) false false))

(event `self.ReceiveBeginPlay`
  (`|ExecutionSequence`
    (:`then_0`
      (bind _outactors (`GameplayStatics.GetAllActorsWithTag` "Red Team")))))

(event `self.Sphere.OnComponentHit`
  (params (HitComponent :type "PrimitiveComponent Object Reference") (OtherActor :type "Actor Object Reference") (OtherComp :type "PrimitiveComponent Object Reference") (NormalImpulse :type "Vector Structure") (Hit :type "HitResult Structure (by ref)"))
  (bind _returnvalue (`SceneComponent.K2_GetComponentLocation` (`self.RadialForce`)))
  (`GameplayStatics.SpawnEmitterAtLocation` "/Game/kosm_fps_assets/Misc/Particles/P_BubbleBurst1.P_BubbleBurst1" (`self.K2_GetActorLocation`) (struct) (4.0 4.0 4.0) :!label _label)
  (`GameplayStatics.ApplyRadialDamage` (`self.DMG value`) (`self.K2_GetActorLocation`) (`self.DMG radius`) null (stale `self.ReceiveBeginPlay` _outactors) self (`self.GetInstigatorController`))
  (`RadialForceComponent.FireImpulse` (`self.RadialForce`))
  (`GameplayStatics.PlaySoundAtLocation` "/Game/AUDIO/SFX_Weapons/Weap_Bubblegun/SC_Energy_Explosion.SC_Energy_Explosion" _returnvalue (struct) 1.0 1.0 0.0 null null null)
  (`GameplayStatics.PlayWorldCameraShake` "/Game/Blueprints/SHAKES/BP_CameraShake_Jump_Heavy.BP_CameraShake_Jump_Heavy_C" _returnvalue 900.0 1000.0)
  (`|SpawnActorFromClass` "/Game/Blueprints/PROJECTILES/BP_BubbleBurst.BP_BubbleBurst_C" (`self.GetTransform`) "Undefined" "OverrideRootScale" null null)
  (`self.K2_DestroyActor`))

(event `CustomEvent_0`
  (bind _returnvalue (`self.K2_GetActorLocation`))
  (bind (_outhit _returnvalue_2) (`KismetSystemLibrary.SphereTraceSingleForObjects` _returnvalue _returnvalue 600.0 (`|MakeArray` "ObjectTypeQuery3" :!type "EObjectTypeQuery Enum") false (`|MakeArray` (`GameplayStatics.GetPlayerCharacter` 0) :!type "Actor Object Reference") "ForOneFrame"))
  (if _returnvalue_2
    _))

(event `self.Sphere.OnComponentBeginOverlap`
  (params (OverlappedComponent :type "PrimitiveComponent Object Reference") (OtherActor :type "Actor Object Reference") (OtherComp :type "PrimitiveComponent Object Reference") (OtherBodyIndex :type Integer) (bFromSweep :type Boolean) (SweepResult :type "HitResult Structure (by ref)"))
  (if (!= OtherActor (`self.GetInstigator`))
    (goto _label)))

(event `self.Sphere1.OnComponentBeginOverlap`
  (params (OverlappedComponent :type "PrimitiveComponent Object Reference") (OtherActor :type "Actor Object Reference") (OtherComp :type "PrimitiveComponent Object Reference") (OtherBodyIndex :type Integer) (bFromSweep :type Boolean) (SweepResult :type "HitResult Structure (by ref)"))
  (bind _projectilemovement (`self.ProjectileMovement`))
  (bind _asep_1_character (cast `/Game/MISSIONS/EP1/Characters/ep1_character` OtherActor))
  (if (not (`/Game/Blueprints/CHARACTERS/NoobotAI/Blueprints/AI_NoobotChar.IsDead?` _asep_1_character))
    (`/Engine/EditorBlueprintResources/StandardMacros.DoOnce` false
      (:`Completed`
        (set `self.Target` _asep_1_character)
        (`KismetSystemLibrary.PrintString` "Hello")
        (set `ProjectileMovementComponent.bIsHomingProjectile` true _projectilemovement)
        (set `MovementComponent.Velocity` (600.0 0.0 0.0) _projectilemovement)
        (set `ProjectileMovementComponent.HomingTargetComponent` (`Character.CapsuleComponent` (`self.Target`)) (`self.ProjectileMovement`))))))

(event `self.ProjectileMovement.OnProjectileBounce`
  (params (ImpactResult :type "HitResult Structure (by ref)") (ImpactVelocity :type "Vector Structure (by ref)"))
  (bind _returnvalue (`self.K2_GetActorLocation`))
  (bind _returnvalue_2 (`SceneComponent.K2_GetComponentLocation` (`self.StaticMesh`)))
  (bind _returnvalue_3 (`SceneComponent.K2_GetComponentLocation` (`self.RadialForce`)))
  (if (== (`self.BounceNumber`) 2.0)
    (`GameplayStatics.SpawnEmitterAtLocation` "/Game/kosm_fps_assets/Misc/Particles/P_BubbleBurst1.P_BubbleBurst1" _returnvalue (struct) (4.0 4.0 4.0))
    (`GameplayStatics.ApplyRadialDamage` (`self.DMG value`) _returnvalue (`self.DMG radius`) null (stale `self.ReceiveBeginPlay` _outactors) self (`self.GetInstigatorController`))
    (`RadialForceComponent.FireImpulse` (`self.RadialForce`))
    (`GameplayStatics.PlaySoundAtLocation` "/Game/AUDIO/SFX_Weapons/Weap_Bubblegun/SC_Energy_Explosion.SC_Energy_Explosion" _returnvalue_2 (struct) 1.0 1.0 0.0 null null null)
    (`GameplayStatics.PlayWorldCameraShake` "/Game/Blueprints/SHAKES/BP_CameraShake_Jump_Heavy.BP_CameraShake_Jump_Heavy_C" _returnvalue_2 900.0 1000.0)
    (`|SpawnActorFromClass` "/Game/Blueprints/PROJECTILES/BP_BubbleBurst.BP_BubbleBurst_C" (`self.GetTransform`) "Undefined" "OverrideRootScale" null null)
    (`self.K2_DestroyActor`)
    (else
      (`GameplayStatics.PlaySoundAtLocation` "/Game/AUDIO/SFX_Weapons/Weap_Bubblegun/SC_Energy_Bounce.SC_Energy_Bounce" _returnvalue_3 (struct) 1.5 1.0 0.0 null null null)
      (set `self.BounceNumber` (+ (`self.BounceNumber`) 1.0))
      (`GameplayStatics.SpawnEmitterAtLocation` "/Game/kosm_fps_assets/Misc/Particles/P_BubbleBurst1_1.P_BubbleBurst1_1" _returnvalue_3 (struct :`Pitch` 90.0 :`Roll` 4905.0) (2.0 1.0 2.0)))))

(fn `UserConstructionScript`)