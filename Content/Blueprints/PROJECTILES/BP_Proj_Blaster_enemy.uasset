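; Enemy blaster projectile that launches with random spread and deals small radial damage on its first hit, sparing the instigator.
; On BeginPlay it sets the beam source, disables physics simulation unless a forward trace finds a portal, and enables CCD after a brief delay.
; On hit it sets the beam target, spawns burst, impact and sound effects, then destroys itself.
; Non-movable components also get crater decals, plus blood effects for Characters.
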(event `self.ReceiveBeginPlay`
  (bind _collisioncomponent (`self.CollisionComponent`))
  (bind _spread (`self.Spread`))
  (bind _projectile (`self.Projectile`))
  (bind _returnvalue (`SceneComponent.K2_GetComponentLocation` _collisioncomponent))
  ;[0.3687 0.5739 1] Begin Play / Apply Damage / Event Hit / Line Trace
  (`ProjectileMovementComponent.SetVelocityInLocalSpace` _projectile (`KismetMathLibrary.MakeVector` 10000.0 (`KismetMathLibrary.RandomFloatInRange` (* _spread -1.0) _spread) (`KismetMathLibrary.RandomFloatInRange` (* _spread -1.0) _spread)))
  (set `ProjectileMovementComponent.bRotationFollowsVelocity` true _projectile)
  (`ParticleSystemComponent.SetBeamSourcePoint` (`self.ParticleSystem`) 0 (`self.K2_GetActorLocation`) 0)
  (`|ExecutionSequence`
    (:`then_0`
      (bind _outactors (`GameplayStatics.GetAllActorsWithTag` "Character"))
      (bind _outactors_2 (`GameplayStatics.GetAllActorsWithTag` "Projectile"))
      (`KismetArrayLibrary.Array_Append` _outactors_2 _outactors)
      (bind _outhit (`KismetSystemLibrary.LineTraceSingle` _returnvalue (+ _returnvalue (* (`KismetMathLibrary.GetForwardVector` (`SceneComponent.K2_GetComponentRotation` _collisioncomponent)) 100000.0)) "TraceTypeQuery1" false _outactors_2))
      (if (not (`.bSuccess` (cast `/Game/kosm_fps_assets/Misc/Portal/PortalBP` (`.HitActor` (`GameplayStatics.BreakHitResult` _outhit)) :!pure true)))
        (`PrimitiveComponent.SetSimulatePhysics` (`self.CollisionComponent`) false)))
    (:`then_1`
      (`KismetSystemLibrary.Delay` 0.02)
      (`PrimitiveComponent.SetUseCCD` (`self.CollisionComponent`) true "None"))))

(event `self.ReceiveHit`
  (params (MyComp :type "PrimitiveComponent Object Reference") (Other :type "Actor Object Reference") (OtherComp :type "PrimitiveComponent Object Reference") (bSelfMoved :type Boolean) (HitLocation :type "Vector Structure") (HitNormal :type "Vector Structure") (NormalImpulse :type "Vector Structure") (Hit :type "HitResult Structure (by ref)"))
  (bind _returnvalue (`self.K2_GetActorLocation`))
  (bind (_bblockinghit _binitialoverlap _time _distance _location _impactpoint _normal _impactnormal _physmat _hitactor) (`GameplayStatics.BreakHitResult` Hit))
  (bind _returnvalue_2 (`KismetMathLibrary.InverseTransformLocation` (`SceneComponent.K2_GetComponentToWorld` OtherComp) HitLocation))
  (bind _returnvalue_3 (`KismetMathLibrary.Conv_VectorToRotator` _normal))
  (bind _returnvalue_4 (`KismetMathLibrary.MakeTransform` (0.0 0.0 0.0) _returnvalue_3))
  ;[0.3687 0.5739 1] Begin Play / Apply Damage / Event Hit / Line Trace
  (`/Engine/EditorBlueprintResources/StandardMacros.DoOnce` false
    (:`Completed`
      (`GameplayStatics.ApplyRadialDamage` 15.0 HitLocation 75.0 null (`|MakeArray` (`self.GetInstigator`) :!type "Actor Object Reference") self (`self.GetInstigatorController`) true "ECC_WorldStatic")
      (`|SpawnActorFromClass` "/Game/Blueprints/PROJECTILES/BP_HitBurst.BP_HitBurst_C" (`KismetMathLibrary.MakeTransform` _returnvalue (struct) (0.25 0.25 0.25)) "Undefined" "OverrideRootScale" null (0.0 0.5 0.25) null)
      (`GameplayStatics.SpawnEmitterAtLocation` "/Game/kosm_fps_assets/Misc/Particles/P_BlasterImpact.P_BlasterImpact" _returnvalue (struct) (8.0 8.0 8.0))
      (`ParticleSystemComponent.SetBeamTargetPoint` (`self.ParticleSystem`) 0 _returnvalue 0)
      (`GameplayStatics.PlaySoundAtLocation` "/Game/AUDIO/SFX_Weapons/Weap_Robots/SC_R-Frame_Ricochet.SC_R-Frame_Ricochet" (`SceneComponent.K2_GetComponentLocation` (`self.RadialForce`)) (struct) 0.2 1.0 0.0 null null null)
      (`|ExecutionSequence`
        (:`then_0`
          (if (not (`|EnumEquality` (`SceneComponent.Mobility` OtherComp) "Movable"))
            (bind _returnvalue_5 (`GameplayStatics.SpawnDecalAttached` "/Game/kosm_fps_assets/Misc/Materials/D_Crater.D_Crater" (7.0 7.0 7.0) OtherComp "None" _returnvalue_2 _returnvalue_3 "SnapToTargetIncludingScale" 5.0))
            (`DecalComponent.SetFadeScreenSize` _returnvalue_5 0.001)
            (if (`.bSuccess` (cast `Character` _hitactor :!pure true))
              (bind _returnvalue_6 (`GameplayStatics.SpawnDecalAtLocation` "/Game/kosm_fps_assets/Misc/Materials/D_BloodStain.D_BloodStain" (`KismetMathLibrary.MakeVector` (`KismetMathLibrary.RandomFloatInRange` 5.0 30.0) (`KismetMathLibrary.RandomFloatInRange` 5.0 30.0) (`KismetMathLibrary.RandomFloatInRange` 5.0 30.0)) _location (`KismetMathLibrary.MakeRotator` (`KismetMathLibrary.RandomFloatInRange` (.roll (.rotation _returnvalue_4)) 360.0) (.pitch (.rotation _returnvalue_4)) (.yaw (.rotation _returnvalue_4)))))
              (`DecalComponent.SetFadeScreenSize` _returnvalue_6 0.001)
              (`GameplayStatics.SpawnEmitterAttached` "/Game/kosm_fps_assets/Misc/Particles/PS_Blood_BulletHit.PS_Blood_BulletHit" OtherComp "None" _returnvalue_2 _returnvalue_3 (0.5 0.5 0.5))))
          (`self.K2_DestroyActor`))
        (:`then_1`
          (`/Engine/EditorBlueprintResources/StandardMacros.IsValid` null))))))

(fn `IgnoreActorWhenMoving`
  (`PrimitiveComponent.IgnoreActorWhenMoving` (`self.CollisionComponent`) (`self.GetInstigator`) true))

(fn `UserConstructionScript`
  (`self.IgnoreActorWhenMoving`))