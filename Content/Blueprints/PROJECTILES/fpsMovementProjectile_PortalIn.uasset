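; Projectile that places the entry portal by moving the Portal1-tagged actor to its impact point, aligned to the surface normal.
; On spawn it traces forward, disables physics simulation unless a PortalBP is hit, and enables CCD after a brief delay.
; Hits ignore characters, barrels, balls, jump pads and pickups.
; Placement assigns scene-capture materials, using a no-target variant while Portal2 is hidden, otherwise refreshing both portals as linked.
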(event `self.ReceiveBeginPlay`
  (bind _collisioncomponent (`self.CollisionComponent`))
  (bind _returnvalue (`SceneComponent.K2_GetComponentLocation` _collisioncomponent))
  ;[0.3687 0.5739 1] Begin Play / Apply Damage / Event Hit / Line Trace
  (`|ExecutionSequence`
    (:`then_0`
      (bind _outactors (`GameplayStatics.GetAllActorsWithTag` "Character"))
      (bind _outactors_2 (`GameplayStatics.GetAllActorsWithTag` "Projectile"))
      (`KismetArrayLibrary.Array_Append` _outactors_2 _outactors)
      (bind _outhit (`KismetSystemLibrary.LineTraceSingle` _returnvalue (+ _returnvalue (* (`KismetMathLibrary.GetForwardVector` (`SceneComponent.K2_GetComponentRotation` _collisioncomponent)) 100000.0)) "TraceTypeQuery1" false _outactors_2))
      (if (not (`.bSuccess` (cast `/Game/kosm_fps_assets/Misc/Portal/PortalBP` (`.HitActor` (`GameplayStatics.BreakHitResult` _outhit)) :!pure true)))
        (`PrimitiveComponent.SetSimulatePhysics` (`self.CollisionComponent`) false)))
    (:`then_1`
      (`KismetSystemLibrary.Delay` 0.02)
      (`PrimitiveComponent.SetUseCCD` (`self.CollisionComponent`) true "None"))))

(event `self.ReceiveHit`
  (params (MyComp :type "PrimitiveComponent Object Reference") (Other :type "Actor Object Reference") (OtherComp :type "PrimitiveComponent Object Reference") (bSelfMoved :type Boolean) (HitLocation :type "Vector Structure") (HitNormal :type "Vector Structure") (NormalImpulse :type "Vector Structure") (Hit :type "HitResult Structure (by ref)"))
  ;[0.3687 0.5739 1] Begin Play / Apply Damage / Event Hit / Line Trace
  (bind _outactors (`GameplayStatics.GetAllActorsWithTag` "Portal1"))
  (if (not (or (`.bSuccess` (cast `Character` Other :!pure true)) (`.bSuccess` (cast `/Game/Blueprints/PHYSICSOBJECTS/PhysicsActor_BarrelBP` Other :!pure true)) (`.bSuccess` (cast `/Game/Blueprints/PHYSICSOBJECTS/PhysicsActor_BallBP` Other :!pure true)) (`.bSuccess` (cast `/Game/Blueprints/JUMPPAD/JumpPad_BP` Other :!pure true)) (`self.ActorHasTag` Other "Pickup")))
    (`/Engine/EditorBlueprintResources/StandardMacros.DoOnce` false
      (:`Completed`
        (`GameplayStatics.PlaySoundAtLocation` "/Game/AUDIO/portalspawn_Cue.portalspawn_Cue" (`SceneComponent.K2_GetComponentLocation` (`self.ParticleSystem`)) (struct) 0.75 1.0 0.0 null null null)
        (bind _output (`|GetArrayItem` _outactors))
        (`self.K2_SetActorLocationAndRotation` _output HitLocation (`KismetMathLibrary.Conv_VectorToRotator` (`.ImpactNormal` (`GameplayStatics.BreakHitResult` Hit))) false true)
        (bind _outactors_2 (`GameplayStatics.GetAllActorsWithTag` "Portal2"))
        (bind _output_2 (`|GetArrayItem` _outactors_2))
        (if (`Actor.bHidden` _output_2)
          (`self.SetActorHiddenInGame` _output false)
          (bind _asportal_bp (cast `/Game/kosm_fps_assets/Misc/Portal/PortalBP` _output :!pure true))
          (bind _portalmeshnear (`/Game/kosm_fps_assets/Misc/Portal/PortalBP.PortalMeshNear` _asportal_bp))
          (bind _returnvalue (`PrimitiveComponent.CreateDynamicMaterialInstance` _portalmeshnear 0 "/Game/kosm_fps_assets/Misc/Materials/PortalIn_RT_NoTarget_Mat_Inst.PortalIn_RT_NoTarget_Mat_Inst" "None"))
          (bind _portalscenecapture (`/Game/kosm_fps_assets/Misc/Portal/PortalBP.PortalSceneCapture` _asportal_bp))
          (bind _texturetarget (`SceneCaptureComponent2D.TextureTarget` _portalscenecapture))
          (`MaterialInstanceDynamic.SetTextureParameterValue` _returnvalue "texture" _texturetarget)
          (`PrimitiveComponent.SetMaterial` (`/Game/kosm_fps_assets/Misc/Portal/PortalBP.PortalMeshFar` _asportal_bp) 0 _returnvalue)
          (`PrimitiveComponent.SetMaterial` (`/Game/kosm_fps_assets/Misc/Portal/PortalBP.PortalMeshInvCube` _asportal_bp) 0 _returnvalue)
          (set `/Game/kosm_fps_assets/Misc/Portal/PortalBP.PortalMaterial` _returnvalue _asportal_bp)
          (`/Game/kosm_fps_assets/Misc/Portal/PortalBP.SetCurrentMipLevel` _asportal_bp 0 _portalscenecapture)
          (bind _asportal_bp_2 (cast `/Game/kosm_fps_assets/Misc/Portal/PortalBP` _output_2 :!pure true))
          (set `/Game/kosm_fps_assets/Misc/Portal/PortalBP.HasTargetPortal` true _asportal_bp_2)
          (set `/Game/kosm_fps_assets/Misc/Portal/PortalBP.HasTargetPortal` true _asportal_bp_2)
          (else
            (`self.SetActorHiddenInGame` _output false)
            (bind _returnvalue_2 (`PrimitiveComponent.CreateDynamicMaterialInstance` _portalmeshnear 0 "/Game/kosm_fps_assets/Misc/Materials/PortalIn_RT_Mat_Inst.PortalIn_RT_Mat_Inst" "None"))
            (`MaterialInstanceDynamic.SetTextureParameterValue` _returnvalue_2 "texture" _texturetarget)
            (`PrimitiveComponent.SetMaterial` (`/Game/kosm_fps_assets/Misc/Portal/PortalBP.PortalMeshInvCube` _asportal_bp) 0 null)
            (`PrimitiveComponent.SetMaterial` (`/Game/kosm_fps_assets/Misc/Portal/PortalBP.PortalMeshFar` _asportal_bp) 0 null)
            (set `/Game/kosm_fps_assets/Misc/Portal/PortalBP.PortalMaterial` _returnvalue_2 _asportal_bp)
            (`/Game/kosm_fps_assets/Misc/Portal/PortalBP.SetCurrentMipLevel` _asportal_bp 0 _portalscenecapture)
            (`self.SetActorHiddenInGame` false)
            (bind _returnvalue_3 (`PrimitiveComponent.CreateDynamicMaterialInstance` (`/Game/kosm_fps_assets/Misc/Portal/PortalBP.PortalMeshNear` _asportal_bp_2) 0 "/Game/kosm_fps_assets/Misc/Materials/PortalOut_RT_Mat_Inst.PortalOut_RT_Mat_Inst" "None"))
            (bind _portalscenecapture_2 (`/Game/kosm_fps_assets/Misc/Portal/PortalBP.PortalSceneCapture` _asportal_bp_2))
            (`MaterialInstanceDynamic.SetTextureParameterValue` _returnvalue_3 "texture" (`SceneCaptureComponent2D.TextureTarget` _portalscenecapture_2))
            (`PrimitiveComponent.SetMaterial` (`/Game/kosm_fps_assets/Misc/Portal/PortalBP.PortalMeshInvCube` _asportal_bp_2) 0 null)
            (`PrimitiveComponent.SetMaterial` (`/Game/kosm_fps_assets/Misc/Portal/PortalBP.PortalMeshFar` _asportal_bp_2) 0 null)
            (set `/Game/kosm_fps_assets/Misc/Portal/PortalBP.PortalMaterial` _returnvalue_3 _asportal_bp_2)
            (`/Game/kosm_fps_assets/Misc/Portal/PortalBP.SetCurrentMipLevel` _asportal_bp_2 0 _portalscenecapture_2)
            (set `/Game/kosm_fps_assets/Misc/Portal/PortalBP.HasTargetPortal` true _asportal_bp_2)
            (set `/Game/kosm_fps_assets/Misc/Portal/PortalBP.HasTargetPortal` true _asportal_bp))))))
  (`self.K2_DestroyActor`))

(fn `IgnoreActorWhenMoving`
  (`PrimitiveComponent.IgnoreActorWhenMoving` (`self.CollisionComponent`) (`self.GetInstigator`) true))

(fn `UserConstructionScript`
  (`self.IgnoreActorWhenMoving`))