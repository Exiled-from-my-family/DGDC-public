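; BP_CEO_AOE2 is an area-of-effect burst that damages the player character with an expanding sphere, then destroys itself.
; On spawn, the Burst timeline grows the sphere while fading it out and ramps up the opacity of a fire-material plane.
; The first overlap with a living fpsMovementCharacter applies damage once and plays a punch camera shake.
; The construction script creates both dynamic materials and tints the plane with the Color variable.
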(event `self.ReceiveBeginPlay`
  (bind _sphere (`self.Sphere`))
  (bind (_direction _newtrack_0) (`Timeline|Burst` :!via `PlayFromStart`)
    (:`Update`
      (`MeshComponent.SetScalarParameterValueOnMaterials` _sphere "opacity" (`KismetMathLibrary.Lerp` 0.25 0.0 _newtrack_0))
      (`SceneComponent.SetRelativeScale3D` _sphere (`KismetMathLibrary.VLerp` (2.0 2.0 2.0) (60.0 60.0 60.0) _newtrack_0))
      (`MeshComponent.SetScalarParameterValueOnMaterials` (`self.Plane`) "Opacity" (`KismetMathLibrary.Lerp` 0.0 16.0 _newtrack_0)))
    (:`Finished`
      (`self.K2_DestroyActor`))))

(event `self.Sphere.OnComponentBeginOverlap`
  (params (OverlappedComponent :type "PrimitiveComponent Object Reference") (OtherActor :type "Actor Object Reference") (OtherComp :type "PrimitiveComponent Object Reference") (OtherBodyIndex :type Integer) (bFromSweep :type Boolean) (SweepResult :type "HitResult Structure (by ref)"))
  (bind _asfps_movement_character_light_1_vq_3 (cast `/Game/Blueprints/CHARACTERS/fpsMovementCharacter_light_1_vq3` OtherActor))
  (if (not (`/Game/Blueprints/CHARACTERS/fpsMovementCharacter_light_1_vq3.IsDead?` _asfps_movement_character_light_1_vq_3))
    (`/Engine/EditorBlueprintResources/StandardMacros.DoOnce` false
      (:`Completed`
        (`GameplayStatics.ApplyDamage` _asfps_movement_character_light_1_vq_3 25.0)
        (`PlayerCameraManager.PlayCameraShake` :`self` (`GameplayStatics.GetPlayerCameraManager` 0) :`ShakeClass` "/Game/Blueprints/SHAKES/BP_CameraShake_Punch.BP_CameraShake_Punch_C")))))

(fn `UserConstructionScript`
  (bind _plane (`self.Plane`))
  (bind _sphere (`self.Sphere`))
  (`PrimitiveComponent.CreateDynamicMaterialInstance` _sphere 0 "/Game/MATERIALS/M_vegasLight_Inst4.M_vegasLight_Inst4" "None")
  (`MeshComponent.SetScalarParameterValueOnMaterials` _sphere "opacity" 1.0)
  (`PrimitiveComponent.CreateDynamicMaterialInstance` _plane 0 "/Game/Blueprints/PICKUPS/M_Fire3_Inst.M_Fire3_Inst" "None")
  (`MeshComponent.SetScalarParameterValueOnMaterials` _plane "Opacity" 1.0)
  (`MeshComponent.SetVectorParameterValueOnMaterials` _plane "Color" (`self.Color`)))