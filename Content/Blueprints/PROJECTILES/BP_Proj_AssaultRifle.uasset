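; Assault rifle projectile that draws a beam tracer from the shooter's muzzle and deals small-radius damage on impact.
; BeginPlay sets the beam source from either player character type or the AI bot, then destroys the actor on non-authority instances.
; The first hit applies damage, ends the beam, adds a bullet-hole decal on non-projectile actors, and destroys itself shortly after; ricochet effects are disabled.
; Construction makes collision ignore the instigator.
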(event `self.ReceiveBeginPlay`
  (bind _returnvalue (`self.GetInstigator`))
  (bind _particlesystem (`self.ParticleSystem`))
  (bind (_asfps_movement_character_light_1_vq_3 _bsuccess) (cast `/Game/Blueprints/CHARACTERS/fpsMovementCharacter_light_1_vq3` _returnvalue :!pure true))
  (bind (_asfps_movement_character_light_2_cpma _bsuccess_2) (cast `/Game/Blueprints/CHARACTERS/fpsMovementCharacter_light_2_cpma` _returnvalue :!pure true))
  (if _bsuccess
    (`ParticleSystemComponent.SetBeamSourcePoint` (`self.ParticleSystem`) 0 (`SceneComponent.K2_GetComponentLocation` (`/Game/Blueprints/CHARACTERS/fpsMovementCharacter_light_1_vq3.Muzzle1P` _asfps_movement_character_light_1_vq_3)) 0)
    (elif _bsuccess_2
      (`ParticleSystemComponent.SetBeamSourcePoint` _particlesystem 0 (`SceneComponent.K2_GetComponentLocation` (`/Game/Blueprints/CHARACTERS/fpsMovementCharacter_light_2_cpma.Muzzle1P` _asfps_movement_character_light_2_cpma)) 0)
      (else
        (bind _asai_noobot_char (cast `/Game/Blueprints/CHARACTERS/NoobotAI/Blueprints/AI_NoobotChar` _returnvalue))
        (`ParticleSystemComponent.SetBeamSourcePoint` _particlesystem 0 (`SceneComponent.K2_GetComponentLocation` (`/Game/Blueprints/CHARACTERS/NoobotAI/Blueprints/AI_NoobotChar.WeaponMuzzle` _asai_noobot_char)) 0))))
  (`/Engine/EditorBlueprintResources/ActorMacros.Switch Has Authority`
    (:`Remote`
      (`self.K2_DestroyActor`))))

(event `self.ReceiveHit`
  (params (MyComp :type "PrimitiveComponent Object Reference") (Other :type "Actor Object Reference") (OtherComp :type "PrimitiveComponent Object Reference") (bSelfMoved :type Boolean) (HitLocation :type "Vector Structure") (HitNormal :type "Vector Structure") (NormalImpulse :type "Vector Structure") (Hit :type "HitResult Structure (by ref)"))
  (bind (_bblockinghit _binitialoverlap _time _distance _location _impactpoint _normal _impactnormal _physmat _hitactor _hitcomponent) (`GameplayStatics.BreakHitResult` Hit))
  ;[0.3687 0.5739 1] Begin Play / Apply Damage / Event Hit / Line Trace
  (`/Engine/EditorBlueprintResources/StandardMacros.DoOnce` false
    (:`Completed`
      (if true
        (`GameplayStatics.ApplyRadialDamage` :`BaseDamage` 9.0 :`Origin` HitLocation :`DamageRadius` 5.0 :`DamageCauser` self :`InstigatedByController` (`self.GetInstigatorController`) :`bDoFullDamage` true)
        (else
          (`GameplayStatics.PlaySoundAtLocation` "/Game/AUDIO/SFX_Weapons/Weap_Minigun/SC_Minigun_Ricochet.SC_Minigun_Ricochet" HitLocation (struct) 1.0 1.0 0.0 null null null)
          (`GameplayStatics.SpawnEmitterAtLocation` "/Game/kosm_fps_assets/Misc/Particles/P_MinigunImpact.P_MinigunImpact" (`self.K2_GetActorLocation`))))
      (`ParticleSystemComponent.SetBeamTargetPoint` (`self.ParticleSystem`) 0 (`self.K2_GetActorLocation`) 0)
      (`/Engine/EditorBlueprintResources/StandardMacros.IsValid` _hitactor
        (:`Is Valid`
          (if (not (`self.ActorHasTag` _hitactor "Projectile"))
            (bind _returnvalue (`GameplayStatics.SpawnDecalAttached` "/Game/kosm_fps_assets/Misc/Materials/BulletHole001.BulletHole001" (10.0 10.0 10.0) OtherComp "None" (`KismetMathLibrary.InverseTransformLocation` (`SceneComponent.K2_GetComponentToWorld` OtherComp) HitLocation) (`KismetMathLibrary.Conv_VectorToRotator` _normal) "KeepRelativeOffset" 30.0))
            (`/Engine/EditorBlueprintResources/StandardMacros.IsValid` _returnvalue
              (:`Is Valid`
                (`DecalComponent.SetFadeScreenSize` _returnvalue 0.001))
              (:`Is Not Valid`
                _)))
          (`KismetSystemLibrary.Delay` 0.5)
          (`self.K2_DestroyActor`))))))

(fn `IgnoreActorWhenMoving`
  (`PrimitiveComponent.IgnoreActorWhenMoving` (`self.CollisionComponent`) (`self.GetInstigator`) true))

(fn `UserConstructionScript`
  (`self.IgnoreActorWhenMoving`))