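; Homing projectile that tracks the player's first-person camera and explodes with radial damage, impulse, sound and camera shake.
; Sphere collision stays off briefly after spawn, then detonates the projectile on a hit or on overlap with anything but its instigator.
; Bounces are counted until one triggers a bubble-burst explosion that also spawns BP_BubbleBurst.
; After a fixed lifetime it self-destructs with effects only, dealing no damage.
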(event `self.ReceiveTick`
  (params (DeltaSeconds :type "Float (single-precision)")))

(event `self.ReceiveBeginPlay`
  (bind _returnvalue (`self.K2_GetActorLocation`))
  (bind _sphere (`self.Sphere`))
  (`|ExecutionSequence`
    (:`then_0`
      (bind _player (`/Game/Blueprints/NewFunctionLibrary.get player`))
      (set `self.Target` _player)
      (set `ProjectileMovementComponent.bIsHomingProjectile` true (`self.ProjectileMovement`))
      (set `ProjectileMovementComponent.HomingTargetComponent` (`/Game/Blueprints/CHARACTERS/fpsMovementCharacter_light_1_vq3.FirstPersonCamera` (`self.Target`)) (`self.ProjectileMovement`))
      (`KismetSystemLibrary.Delay` 10.0)
      (`GameplayStatics.SpawnEmitterAtLocation` "/Game/kosm_fps_assets/Misc/Particles/P_RailgunBurst.P_RailgunBurst" _returnvalue (struct) (8.0 8.0 8.0))
      (`GameplayStatics.PlaySoundAtLocation` "/Game/AUDIO/SFX_Weapons/Weap_Bubblegun/SC_Energy_Explosion.SC_Energy_Explosion" _returnvalue (struct) 1.0 1.0 0.0 null null null)
      (`GameplayStatics.PlayWorldCameraShake` "/Game/Blueprints/SHAKES/BP_CameraShake_Jump_Heavy.BP_CameraShake_Jump_Heavy_C" _returnvalue 900.0 1000.0)
      (`self.K2_DestroyActor`))
    (:`then_1`
      (`PrimitiveComponent.SetCollisionEnabled` _sphere "NoCollision")
      (`KismetSystemLibrary.Delay` 0.4)
      (`PrimitiveComponent.SetCollisionEnabled` _sphere "QueryAndPhysics"))))

(event `self.Sphere.OnComponentHit`
  (params (HitComponent :type "PrimitiveComponent Object Reference") (OtherActor :type "Actor Object Reference") (OtherComp :type "PrimitiveComponent Object Reference") (NormalImpulse :type "Vector Structure") (Hit :type "HitResult Structure (by ref)"))
  (bind _returnvalue (`SceneComponent.K2_GetComponentLocation` (`self.RadialForce`)))
  (`GameplayStatics.SpawnEmitterAtLocation` "/Game/kosm_fps_assets/Misc/Particles/P_RailgunBurst.P_RailgunBurst" (`self.K2_GetActorLocation`) (struct) (8.0 8.0 8.0) :!label _label)
  (`GameplayStatics.ApplyRadialDamage` :`BaseDamage` (`self.DMG value`) :`Origin` (`self.K2_GetActorLocation`) :`DamageRadius` (`self.DMG radius`) :`DamageCauser` self :`InstigatedByController` (`self.GetInstigatorController`))
  (`RadialForceComponent.FireImpulse` (`self.RadialForce`))
  (`GameplayStatics.PlaySoundAtLocation` "/Game/AUDIO/SFX_Weapons/Weap_Bubblegun/SC_Energy_Explosion.SC_Energy_Explosion" _returnvalue (struct) 1.0 1.0 0.0 null null null)
  (`GameplayStatics.PlayWorldCameraShake` "/Game/Blueprints/SHAKES/BP_CameraShake_Jump_Heavy.BP_CameraShake_Jump_Heavy_C" _returnvalue 900.0 1000.0)
  (`self.K2_DestroyActor`))

(event `self.Sphere.OnComponentBeginOverlap`
  (params (OverlappedComponent :type "PrimitiveComponent Object Reference") (OtherActor :type "Actor Object Reference") (OtherComp :type "PrimitiveComponent Object Reference") (OtherBodyIndex :type Integer) (bFromSweep :type Boolean) (SweepResult :type "HitResult Structure (by ref)"))
  (if (!= OtherActor (`self.GetInstigator`))
    (goto _label)))

(event `self.ProjectileMovement.OnProjectileBounce`
  (params (ImpactResult :type "HitResult Structure (by ref)") (ImpactVelocity :type "Vector Structure (by ref)"))
  (bind _returnvalue (`self.K2_GetActorLocation`))
  (bind _returnvalue_2 (`SceneComponent.K2_GetComponentLocation` (`self.StaticMesh`)))
  (bind _returnvalue_3 (`SceneComponent.K2_GetComponentLocation` (`self.RadialForce`)))
  (if (== (`self.BounceNumber`) 2.0)
    (`GameplayStatics.SpawnEmitterAtLocation` "/Game/kosm_fps_assets/Misc/Particles/P_BubbleBurst1.P_BubbleBurst1" _returnvalue (struct) (4.0 4.0 4.0))
    (`GameplayStatics.ApplyRadialDamage` :`BaseDamage` (`self.DMG value`) :`Origin` _returnvalue :`DamageRadius` (`self.DMG radius`) :`DamageCauser` self :`InstigatedByController` (`self.GetInstigatorController`))
    (`RadialForceComponent.FireImpulse` (`self.RadialForce`))
    (`GameplayStatics.PlaySoundAtLocation` "/Game/AUDIO/SFX_Weapons/Weap_Bubblegun/SC_Energy_Explosion.SC_Energy_Explosion" _returnvalue_2 (struct) 1.0 1.0 0.0 null null null)
    (`GameplayStatics.PlayWorldCameraShake` "/Game/Blueprints/SHAKES/BP_CameraShake_Jump_Heavy.BP_CameraShake_Jump_Heavy_C" _returnvalue_2 900.0 1000.0)
    (`|SpawnActorFromClass` "/Game/Blueprints/PROJECTILES/BP_BubbleBurst.BP_BubbleBurst_C" (`self.GetTransform`) "Undefined" "OverrideRootScale" null null)
    (`self.K2_DestroyActor`)
    (else
      (`GameplayStatics.PlaySoundAtLocation` "/Game/AUDIO/SFX_Weapons/Weap_Bubblegun/SC_Energy_Bounce.SC_Energy_Bounce" _returnvalue_3 (struct) 1.5 1.0 0.0 null null null)
      (set `self.BounceNumber` (+ (`self.BounceNumber`) 1.0))
      (`GameplayStatics.SpawnEmitterAtLocation` "/Game/kosm_fps_assets/Misc/Particles/P_BubbleBurst1_1.P_BubbleBurst1_1" _returnvalue_3 (struct :`Pitch` 90.0 :`Roll` 4905.0) (2.0 1.0 2.0)))))

(fn `UserConstructionScript`)