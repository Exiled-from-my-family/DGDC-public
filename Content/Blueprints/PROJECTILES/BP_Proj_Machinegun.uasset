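; Machine gun bullet fired by an EP4_Security instigator, resolved as a spread-randomised hitscan on BeginPlay behind a launched projectile.
; A line trace sets the tracer beam's target from the muzzle; movable hits take small radial damage, sparing "Gmax"-tagged actors.
; Undead characters get blood spray and a second-trace floor decal; non-movable surfaces get impact effects, ricochet sound and bullet holes.
; Collision hit events are empty, and ricochet respawning is unwired.
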(event `self.ReceiveBeginPlay`
  (bind _collisioncomponent (`self.CollisionComponent`))
  (bind _projectile (`self.Projectile`))
  (bind _spread (`self.Spread`))
  (bind _returnvalue (`SceneComponent.K2_GetComponentLocation` _collisioncomponent))
  (bind _returnvalue_2 (* _spread -1.0))
  (bind (_asep4_security _bsuccess) (cast `/Game/MISSIONS/EP4/Characters/ep4_security` (`self.GetInstigator`) :!pure true))
  (bind _returnvalue_3 (`KismetMathLibrary.RandomFloatInRange` _returnvalue_2 _spread))
  ;[0.3687 0.5739 1] Begin Play / Apply Damage / Event Hit / Line Trace
  (`ProjectileMovementComponent.SetVelocityInLocalSpace` _projectile (`KismetMathLibrary.MakeVector` 10000.0 _returnvalue_3 _returnvalue_3))
  (if _bsuccess
    (`ParticleSystemComponent.SetBeamSourcePoint` (`self.ParticleSystem`) 0 (`SceneComponent.K2_GetComponentLocation` (`/Game/Blueprints/CHARACTERS/NoobotAI/Blueprints/AI_NoobotChar.WeaponMuzzle` _asep4_security)) 0)
    (set `ProjectileMovementComponent.bRotationFollowsVelocity` true _projectile)
    (bind (_outhit _returnvalue_4) (`KismetSystemLibrary.LineTraceSingle` _returnvalue (+ (+ _returnvalue (* (`SceneComponent.GetForwardVector` _collisioncomponent) 8000.0)) (`KismetMathLibrary.MakeVector` _returnvalue_3 (`KismetMathLibrary.RandomFloatInRange` _returnvalue_2 _spread) (`KismetMathLibrary.RandomFloatInRange` _returnvalue_2 _spread))) "TraceTypeQuery1" false (`|MakeArray` (`self.NewVar_0`) (`self.Instigator`) :!type "Actor Object Reference") "None" true (struct :`R` 1.0 :`A` 1.0) (struct :`G` 1.0 :`A` 1.0) 2.0))
    (bind _outactors (`GameplayStatics.GetAllActorsWithTag` "Gmax"))
    (if _returnvalue_4
      (`|ExecutionSequence`
        (:`then_0`
          (bind (_bblockinghit _binitialoverlap _time _distance _location _impactpoint _normal _impactnormal _physmat _hitactor _hitcomponent) (`GameplayStatics.BreakHitResult` _outhit))
          (`ParticleSystemComponent.SetBeamTargetPoint` (`self.ParticleSystem`) 0 _location 0)
          (if (`|EnumEquality` (`SceneComponent.Mobility` _hitcomponent) "Movable")
            (`GameplayStatics.ApplyRadialDamage` 0.0 _location 10.0 null _outactors self (`self.GetInstigatorController`) true)
            (if (and (`self.ActorHasTag` _hitactor "Undead") (`.bSuccess` (cast `Character` _hitactor :!pure true)))
              (bind (_outhit_2 _returnvalue_5) (`KismetSystemLibrary.LineTraceSingle` _location (+ _location (* (`KismetMathLibrary.GetUpVector` (`KismetMathLibrary.FindLookAtRotation` (`self.K2_GetActorLocation`) _location)) -300.0)) "TraceTypeQuery1"))
              (if _returnvalue_5
                (bind (_bblockinghit_2 _binitialoverlap_2 _time_2 _distance_2 _location_2 _impactpoint_2 _normal_2) (`GameplayStatics.BreakHitResult` _outhit_2))
                (bind _returnvalue_6 (`GameplayStatics.SpawnDecalAtLocation` (select `int` (`KismetMathLibrary.RandomIntegerInRange` 0 7) :`0` "/Game/kosm_fps_assets/Misc/Materials/D_BloodStain_Inst.D_BloodStain_Inst" :`1` "/Game/kosm_fps_assets/Misc/Materials/D_BloodStain_Inst1.D_BloodStain_Inst1" :`2` "/Game/kosm_fps_assets/Misc/Materials/D_BloodStain_Inst2.D_BloodStain_Inst2" :`3` "/Game/kosm_fps_assets/Misc/Materials/D_BloodStain_Inst3.D_BloodStain_Inst3" :`4` "/Game/kosm_fps_assets/Misc/Materials/D_BloodStain_Inst4.D_BloodStain_Inst4" :`5` "/Game/kosm_fps_assets/Misc/Materials/D_BloodStain_Inst5.D_BloodStain_Inst5" :`6` "/Game/kosm_fps_assets/Misc/Materials/D_BloodStain_Inst6.D_BloodStain_Inst6" :`7` "/Game/kosm_fps_assets/Misc/Materials/D_BloodStain_Inst7.D_BloodStain_Inst7" :!type "MaterialInterface Object Reference") (`KismetMathLibrary.MakeVector` (`KismetMathLibrary.RandomFloatInRange` 100.0 120.0) (`KismetMathLibrary.RandomFloatInRange` 100.0 120.0) (`KismetMathLibrary.RandomFloatInRange` 100.0 120.0)) _location_2 (`KismetMathLibrary.MakeRotFromX` _normal_2) 10.0))
                (`DecalComponent.SetFadeScreenSize` _returnvalue_6 0.001))
              (bind _returnvalue_7 (`KismetMathLibrary.Conv_VectorToRotator` _normal))
              (`GameplayStatics.SpawnEmitterAtLocation` "/Game/kosm_fps_assets/Misc/Particles/PS_Blood_BulletHit1.PS_Blood_BulletHit1" _location _returnvalue_7)
              (`KismetSystemLibrary.Delay` 0.05 :!label _label)
              (`self.K2_DestroyActor`))
            (else
              (`GameplayStatics.SpawnEmitterAtLocation` "/Game/kosm_fps_assets/Misc/Particles/P_MinigunImpact.P_MinigunImpact" _location (struct) (0.75 0.75 0.75))
              (`GameplayStatics.PlaySoundAtLocation` "/Game/AUDIO/SFX_Weapons/Weap_Minigun/SC_Minigun_Ricochet.SC_Minigun_Ricochet" _location (struct) 1.0 1.0 0.0 null null null)
              (bind _returnvalue_8 (`KismetMathLibrary.InverseTransformLocation` (`SceneComponent.K2_GetComponentToWorld` _hitcomponent) _location))
              (`GameplayStatics.SpawnEmitterAtLocation` null _returnvalue_8 _returnvalue_7 (1.0 100.0 1.0))
              (bind _returnvalue_9 (`GameplayStatics.SpawnDecalAttached` "/Game/kosm_fps_assets/Misc/Materials/BulletHole001.BulletHole001" (4.0 4.0 4.0) _hitcomponent "None" _returnvalue_8 _returnvalue_7 "KeepRelativeOffset" 30.0))
              (`DecalComponent.SetFadeScreenSize` _returnvalue_9 0.001)
              (goto _label))))
        (:`then_1`
          (`KismetSystemLibrary.Delay` (`KismetMathLibrary.RandomFloatInRange` -0.2 0.1) :!label _label_2)
          (`ActorComponent.K2_DestroyComponent` (`self.StaticMesh`))))
      (else
        (goto _label_2)))))

(event `self.ReceiveHit`
  (params (MyComp :type "PrimitiveComponent Object Reference") (Other :type "Actor Object Reference") (OtherComp :type "PrimitiveComponent Object Reference") (bSelfMoved :type Boolean) (HitLocation :type "Vector Structure") (HitNormal :type "Vector Structure") (NormalImpulse :type "Vector Structure") (Hit :type "HitResult Structure (by ref)"))
  ;[0.3687 0.5739 1] Begin Play / Apply Damage / Event Hit / Line Trace
)

(event `self.CollisionComponent.OnComponentHit`
  (params (HitComponent :type "PrimitiveComponent Object Reference") (OtherActor :type "Actor Object Reference") (OtherComp :type "PrimitiveComponent Object Reference") (NormalImpulse :type "Vector Structure") (Hit :type "HitResult Structure (by ref)"))
  ;[0.3687 0.5739 1] Begin Play / Apply Damage / Event Hit / Line Trace
)

(fn `IgnoreActorWhenMoving`
  (`PrimitiveComponent.IgnoreActorWhenMoving` (`self.CollisionComponent`) (`self.GetInstigator`) true))

(fn `UserConstructionScript`
  (`self.IgnoreActorWhenMoving`))