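; Plasma cut beam projectile that acts as a hitscan laser, running one forward line trace on BeginPlay with authority.
; The trace sets the beam particle endpoints, damages Characters lacking the "Red Team" tag while raising the player's PlasmaCharge, and overcharges EP3_robot targets.
; Other hit actors get a lightning emitter at the impact.
; Construction makes it ignore its instigator when moving, and a Hit event destroys it after a short delay.
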(event Custom|Laser_LineTrace
  (params (StartTrace :type Vector :default "0.000000,0.000000,0") (EndTrace :type Vector))
  (bind _particlesystem (Variables|Default|GetParticleSystem))
  (bind _collisioncomponent (Variables|MyProjectile|GetCollisionComponent))
  (bind _collisioncomponent_2 (Variables|MyProjectile|GetCollisionComponent))
  (bind _particlesystem_2 (Variables|Default|GetParticleSystem))
  (bind _returnvalue (Transformation|GetWorldLocation _collisioncomponent))
  (bind _returnvalue_2 (Math|Vector|GetForwardVector _collisioncomponent))
  (bind _returnvalue_3 (Transformation|GetWorldLocation _collisioncomponent_2))
  (bind _returnvalue_4 (* _returnvalue_2 6e+03))
  (bind _returnvalue_5 (+ _returnvalue _returnvalue_4))
  ;[0.3687 0.5739 1] Begin Play / Apply Damage / Event Hit / Line Trace
  (Class|ParticleSystemComponent|SetBeamSourcePoint _particlesystem 0 _returnvalue_3)
  (Class|ParticleSystemComponent|SetBeamSourcePoint _particlesystem 2 _returnvalue_3)
  (Class|ParticleSystemComponent|SetBeamTargetPoint _particlesystem_2 1 _returnvalue_5)
  (Class|ParticleSystemComponent|SetBeamTargetPoint _particlesystem_2 2 _returnvalue_5)
  (bind (_outhit _returnvalue_6) (Collision|LineTraceByChannel StartTrace EndTrace "TraceTypeQuery1" false (Utilities|Array|MakeArray (Variables|Default|GetOwningPawn) (Variables|Actor|GetInstigator)) "None" true "(R=1.000000,G=0.000000,B=0.000000,A=1.000000)" "(R=0.000000,G=1.000000,B=0.000000,A=1.000000)" 2.0))
  (if _returnvalue_6
    (Utilities|IsValid (.HitActor (Collision|BreakHitResult _outhit))
      (:Is%20Valid
        (if (.bSuccess (Utilities|Casting|CastToCharacter (.HitActor (Collision|BreakHitResult _outhit))))
          (if (Actor|ActorHasTag (.HitActor (Collision|BreakHitResult _outhit)) "Red Team")
            _
            (else
              (bind _player (CallFunction|GetPlayer))
              (bind _result (Math|Integer|IncrementInt (Variables|/Game/Blueprints/CHARACTERS/fpsMovementCharacter_light_1_vq3.fpsMovementCharacter_light_1_vq3_C|GetPlasmaCharge _player))
                (:%20%20
                  (Development|PrintString (Utilities|String|ToString(Integer) _result) true false)
                  (Game|Damage|ApplyRadialDamage 4.0 (.Location (Collision|BreakHitResult _outhit)) 1.0 0 0 self (Game|GetInstigatorController) true "ECC_Visibility")))))
          (Utilities|FlowControl|Sequence
            (:then_0
              (bind _asep3_robot (Utilities|Casting|CastToEP3_robot (.HitActor (Collision|BreakHitResult _outhit))))
              (if (stale _bsuccess)
                (Default|Overcharghe _asep3_robot))))
          (else
            (Effects|SpawnEmitteratLocation "/Game/kosm_fps_assets/Misc/Particles/P_Lightning.P_Lightning" (- (.Location (Collision|BreakHitResult _outhit)) (Math|Conversions|ToVector(Float) (Math|Random|RandomFloatinRange -2.0 2.0))))))))))

(event Collision|EventHit
  (params (MyComp :type Primitive%20Component%20Object%20Reference) (Other :type Actor%20Object%20Reference) (OtherComp :type Primitive%20Component%20Object%20Reference) (bSelfMoved :type Boolean) (HitLocation :type Vector :default "0, 0, 0") (HitNormal :type Vector :default "0, 0, 0") (NormalImpulse :type Vector :default "0, 0, 0") (Hit :type Hit%20Result%20Structure%20%28by%20ref%29))
  ;[0.3687 0.5739 1] Begin Play / Apply Damage / Event Hit / Line Trace
  (Utilities|FlowControl|Delay 0.2)
  (Actor|DestroyActor))

(event EventBeginPlay
  (bind _collisioncomponent (Variables|MyProjectile|GetCollisionComponent))
  (bind _returnvalue (Transformation|GetWorldLocation _collisioncomponent))
  (bind _returnvalue_2 (Math|Vector|GetForwardVector _collisioncomponent))
  ;[0.3687 0.5739 1] Begin Play / Apply Damage / Event Hit / Line Trace
  (Networking|SwitchHasAuthority
    (:Authority
      (CallFunction|LaserLineTrace (+ _returnvalue (* _returnvalue_2 1e+02)) (+ _returnvalue (* _returnvalue_2 3e+03))))
    (:Remote
      (Development|PrintString "lghtg remote"))))

(fn ConstructionScript
  (CallFunction|IgnoreActorwhenMoving))

(fn IgnoreActorwhenMoving
  (Collision|IgnoreActorwhenMoving (Variables|MyProjectile|GetCollisionComponent) (Game|GetInstigator) true))