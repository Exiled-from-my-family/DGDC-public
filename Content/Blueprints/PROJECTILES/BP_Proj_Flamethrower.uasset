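; Flamethrower projectile that launches forward with random spread, grows along a timeline and destroys itself after a short lifetime.
; On spawn, a forward trace ignoring characters and projectiles turns off collision physics simulation unless it hits a portal, and CCD is enabled shortly after.
; Overlapping an FPS character applies damage once; the instigator is ignored when moving.
; The Hit event is empty, leaving nailgun-style radial damage, decal and effect logic disconnected.
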(event `self.ReceiveBeginPlay`
  (bind _projectile (`self.Projectile`))
  (bind _spread (`self.Spread`))
  (bind _collisioncomponent (`self.CollisionComponent`))
  (bind _returnvalue (`SceneComponent.K2_GetComponentLocation` _collisioncomponent))
  (bind _returnvalue_2 (* _spread -1.0))
  ;[0.3687 0.5739 1] Begin Play / Apply Damage / Event Hit / Line Trace
  (set `ProjectileMovementComponent.bRotationFollowsVelocity` true _projectile)
  (`ProjectileMovementComponent.SetVelocityInLocalSpace` _projectile (`KismetMathLibrary.MakeVector` 4000.0 (`KismetMathLibrary.RandomFloatInRange` _returnvalue_2 _spread) (`KismetMathLibrary.RandomFloatInRange` _returnvalue_2 _spread)))
  (`|ExecutionSequence`
    (:`then_0`
      (bind _outactors (`GameplayStatics.GetAllActorsWithTag` "Character"))
      (bind _outactors_2 (`GameplayStatics.GetAllActorsWithTag` "Projectile"))
      (`KismetArrayLibrary.Array_Append` _outactors_2 _outactors)
      (bind _outhit (`KismetSystemLibrary.LineTraceSingle` _returnvalue (+ _returnvalue (* (`KismetMathLibrary.GetForwardVector` (`SceneComponent.K2_GetComponentRotation` _collisioncomponent)) 100000.0)) "TraceTypeQuery1" false _outactors_2))
      (if (not (`.bSuccess` (cast `/Game/kosm_fps_assets/Misc/Portal/PortalBP` (`.HitActor` (`GameplayStatics.BreakHitResult` _outhit)) :!pure true)))
        (`PrimitiveComponent.SetSimulatePhysics` (`self.CollisionComponent`) false)))
    (:`then_1`
      (`KismetSystemLibrary.Delay` 0.02)
      (`PrimitiveComponent.SetUseCCD` (`self.CollisionComponent`) true "None"))
    (:`then_2`
      (`KismetSystemLibrary.Delay` 0.75)
      (`self.K2_DestroyActor`))
    (:`then_3`
      (bind (_direction _newtrack_0) (`Timeline|resize` :!via `PlayFromStart`)
        (:`Update`
          (`self.SetActorRelativeScale3D` (`KismetMathLibrary.VLerp` (0.25 0.25 0.25) (2.0 2.0 2.0) _newtrack_0)))))))

(event `self.ReceiveHit`
  (params (MyComp :type "PrimitiveComponent Object Reference") (Other :type "Actor Object Reference") (OtherComp :type "PrimitiveComponent Object Reference") (bSelfMoved :type Boolean) (HitLocation :type "Vector Structure") (HitNormal :type "Vector Structure") (NormalImpulse :type "Vector Structure") (Hit :type "HitResult Structure (by ref)"))
  ;[0.3687 0.5739 1] Begin Play / Apply Damage / Event Hit / Line Trace
)

(event `self.CollisionComponent.OnComponentBeginOverlap`
  (params (OverlappedComponent :type "PrimitiveComponent Object Reference") (OtherActor :type "Actor Object Reference") (OtherComp :type "PrimitiveComponent Object Reference") (OtherBodyIndex :type Integer) (bFromSweep :type Boolean) (SweepResult :type "HitResult Structure (by ref)"))
  ;[0.3687 0.5739 1] Begin Play / Apply Damage / Event Hit / Line Trace
  (bind _asfps_movement_character_light_1_vq_3 (cast `/Game/Blueprints/CHARACTERS/fpsMovementCharacter_light_1_vq3` OtherActor))
  (`/Engine/EditorBlueprintResources/StandardMacros.DoOnce` false
    (:`Completed`
      (`KismetSystemLibrary.PrintString` "burn baby")
      (`GameplayStatics.ApplyDamage` _asfps_movement_character_light_1_vq_3 6.0 null (`self.GetInstigatorController`)))))

(fn `IgnoreActorWhenMoving`
  (`PrimitiveComponent.IgnoreActorWhenMoving` (`self.CollisionComponent`) (`self.GetInstigator`) true))

(fn `UserConstructionScript`
  (`self.IgnoreActorWhenMoving`))