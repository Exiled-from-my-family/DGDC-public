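; Explosive missile projectile, named for robot use, that detonates on a hit or when its proximity sphere overlaps an actor other than the instigator.
; The sphere arms shortly after spawn; hits on non-movable components also spawn a grenade burst and crater decal.
; Both triggers share the explosion path, which skips big robots, applies radial damage only if the Hit actor is the FPS character, fires an impulse, then destroys the missile after a delay.
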(event `self.ReceiveBeginPlay`
  (bind _sphere (`self.Sphere`))
  (`PrimitiveComponent.SetCollisionEnabled` _sphere "NoCollision")
  (`KismetSystemLibrary.Delay` 0.2)
  (`PrimitiveComponent.SetCollisionEnabled` _sphere "QueryAndPhysics"))

(event `self.ReceiveHit`
  (params (MyComp :type "PrimitiveComponent Object Reference") (Other :type "Actor Object Reference") (OtherComp :type "PrimitiveComponent Object Reference") (bSelfMoved :type Boolean) (HitLocation :type "Vector Structure") (HitNormal :type "Vector Structure") (NormalImpulse :type "Vector Structure") (Hit :type "HitResult Structure (by ref)"))
  (bind _returnvalue (`self.GetInstigatorController`))
  (if (`|EnumInequality` (`SceneComponent.Mobility` OtherComp) "Movable")
    (`/Engine/EditorBlueprintResources/StandardMacros.IsValid` OtherComp
      (:`Is Valid`
        (`|SpawnActorFromClass` "/Game/Blueprints/PROJECTILES/BP_GrenadeBurst.BP_GrenadeBurst_C" (`KismetMathLibrary.MakeTransform` (`self.K2_GetActorLocation`) (struct) (1.0 1.0 1.0)) "Undefined" "OverrideRootScale" null null null)
        (`GameplayStatics.SpawnDecalAttached` "/Game/kosm_fps_assets/Misc/Materials/D_Crater.D_Crater" (100.0 100.0 100.0) OtherComp "None" (`KismetMathLibrary.InverseTransformLocation` (`SceneComponent.K2_GetComponentToWorld` OtherComp) HitLocation) (`KismetMathLibrary.Conv_VectorToRotator` HitNormal) "KeepRelativeOffset" 30.0))
      (:`Is Not Valid`
        _)))
  (`GameplayStatics.SpawnEmitterAtLocation` "/Game/kosm_fps_assets/Misc/Particles/P_Explode3.P_Explode3" (`self.K2_GetActorLocation`) (struct) (4.0 4.0 4.0) :!label _label)
  (if (not (`.bSuccess` (cast `/Game/MISSIONS/EP3/Characters/EP3_robot_big` Other :!pure true)))
    (if (`.bSuccess` (cast `/Game/Blueprints/CHARACTERS/fpsMovementCharacter_light_1_vq3` Other :!pure true))
      (`GameplayStatics.ApplyRadialDamage` 65.0 (`self.K2_GetActorLocation`) 800.0 null (`|MakeArray` _returnvalue :!type "Actor Object Reference") self _returnvalue))
    (`RadialForceComponent.FireImpulse` (`self.RadialForce`))
    (`ActorComponent.K2_DestroyComponent` (`self.RadialForce`))
    (`SceneComponent.SetHiddenInGame` (`self.StaticMesh`) true false)
    (`self.SetActorEnableCollision` false)
    (`GameplayStatics.PlaySoundAtLocation` "/Game/AUDIO/SFX_Weapons/Weap_GrenadeLauncher/SC_Explosion.SC_Explosion" (`self.K2_GetActorLocation`) (struct) 1.0 1.0 0.0 null null null))
  (`KismetSystemLibrary.Delay` 1.5)
  (`self.K2_DestroyActor`))

(event `self.Sphere.OnComponentBeginOverlap`
  (params (OverlappedComponent :type "PrimitiveComponent Object Reference") (OtherActor :type "Actor Object Reference") (OtherComp :type "PrimitiveComponent Object Reference") (OtherBodyIndex :type Integer) (bFromSweep :type Boolean) (SweepResult :type "HitResult Structure (by ref)"))
  (if (!= OtherActor (`self.GetInstigator`))
    (goto _label)))

(event `self.ProjectileMovement.OnProjectileBounce`
  (params (ImpactResult :type "HitResult Structure (by ref)") (ImpactVelocity :type "Vector Structure (by ref)"))
  (`GameplayStatics.PlaySoundAtLocation` "/Game/AUDIO/SFX_Weapons/Weap_GrenadeLauncher/SC_GrenadeHit.SC_GrenadeHit" (`self.K2_GetActorLocation`) (struct) 1.0 1.0 0.0 null null null))

(fn `UserConstructionScript`)