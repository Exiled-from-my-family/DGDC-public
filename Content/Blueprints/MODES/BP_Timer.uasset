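; BP_Timer is the match countdown actor, starting from the game instance's time limit and showing minutes and seconds in a W_Timer widget.
; Tick feeds a one-second Delay to count down while unpaused, with a one-time color change, message and alarm at the RemainingTime threshold.
; At zero it calls TIMEOUT once and removes the widget, unless BP_ArcadeGameMode reports the match already ended.
; Player respawn recreates the widget from current values.
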(event `self.ReceiveBeginPlay`
  (bind _game_instance (`/Game/Blueprints/NewFunctionLibrary.dead game instance`))
  (set `self.Value minutes` (- (`/Game/Blueprints/DeadGaemInstance.time limit` _game_instance) 1))
  (bind _asfps_movement_character_light_1_vq_3 (cast `/Game/Blueprints/CHARACTERS/fpsMovementCharacter_light_1_vq3` (`GameplayStatics.GetPlayerPawn` 0)))
  (add `/Game/Blueprints/CHARACTERS/fpsMovementCharacter_light_1_vq3.respawned` _asfps_movement_character_light_1_vq_3 (delegate `redoscore`))
  (bind _returnvalue (`|CreateWidget` "/Game/Blueprints/UI/UI_Arcade/W_Timer.W_Timer_C" (`GameplayStatics.GetPlayerController` 0)))
  (bind _output_get (set `self.UI` _returnvalue))
  (bind _game_instance_2 (`/Game/Blueprints/NewFunctionLibrary.dead game instance`))
  (set `/Game/Blueprints/UI/UI_Arcade/W_Timer.Minutes text` (`KismetTextLibrary.Conv_IntToText` (- (`/Game/Blueprints/DeadGaemInstance.time limit` _game_instance_2) 1)) _output_get)
  (`UserWidget.AddToViewport` _returnvalue 0))

(event `redoscore`
  (bind _ui (`self.UI`))
  (bind _returnvalue (`|CreateWidget` "/Game/Blueprints/UI/UI_Arcade/W_Timer.W_Timer_C" (`GameplayStatics.GetPlayerController` 0)))
  (set `self.UI` _returnvalue)
  (`UserWidget.AddToViewport` _returnvalue 0)
  (bind _output_get (set `/Game/Blueprints/UI/UI_Arcade/W_Timer.Seconds num` (`self.Value seconds`) _ui))
  (set `/Game/Blueprints/UI/UI_Arcade/W_Timer.Seconds text` (`KismetTextLibrary.Conv_IntToText` _output_get) _ui)
  (bind _output_get_2 (set `/Game/Blueprints/UI/UI_Arcade/W_Timer.Minutes num` (`self.Value minutes`) _ui))
  (set `/Game/Blueprints/UI/UI_Arcade/W_Timer.Minutes text` (`KismetTextLibrary.Conv_IntToText` _output_get_2) _ui))

(event `self.ReceiveTick`
  (params (DeltaSeconds :type "Float (single-precision)"))
  (bind _ui (`self.UI`))
  (bind _text_color (`/Game/Blueprints/UI/UI_Arcade/W_Timer.Text color` (`self.UI`)))
  (`KismetSystemLibrary.Delay` 1.0)
  ;[1 1 1] If game is paused timer stops
  (if (`GameplayStatics.IsGamePaused`)
    _
    (elif (== (`self.Value seconds`) 0)
      (if (== (`self.Value minutes`) 0)
        ;[1 1 1] if match already ended the timeout doesn't get called
        (bind _outactors (`GameplayStatics.GetAllActorsOfClass` "/Game/Blueprints/MODES/BP_ArcadeGameMode.BP_ArcadeGameMode_C"))
        (if (not (`/Game/Blueprints/MODES/BP_ArcadeGameMode.MATCH ALREADY ENDED?` (`|GetArrayItem` _outactors)))
          (`/Engine/EditorBlueprintResources/StandardMacros.DoOnce` false
            (:`Completed`
              (`self.TIME OUT`)
              (`Widget.RemoveFromParent` (`self.UI`)))))
        (else
          (bind _output_get (set `self.Value seconds` 59))
          (set `/Game/Blueprints/UI/UI_Arcade/W_Timer.Seconds text` (`KismetTextLibrary.Conv_IntToText` _output_get) (`self.UI`))
          (bind _output_get_2 (set `self.Value minutes` (- (`self.Value minutes`) 1)))
          (set `/Game/Blueprints/UI/UI_Arcade/W_Timer.Minutes text` (`KismetTextLibrary.Conv_IntToText` _output_get_2) (`self.UI`))
          (if (== (`self.Value minutes`) (`self.Remaining time`))
            (`/Engine/EditorBlueprintResources/StandardMacros.DoOnce` false
              (:`Completed`
                (`TextBlock.SetColorAndOpacity` (`/Game/Blueprints/UI/UI_Arcade/W_Timer.TEXTMinutes` _ui) _text_color)
                (`TextBlock.SetColorAndOpacity` (`/Game/Blueprints/UI/UI_Arcade/W_Timer.TEXTSeconds` _ui) _text_color)
                (bind _returnvalue (`|CreateWidget` "/Game/Blueprints/UI/UI_Pickups/UI_GenericMessage.UI_GenericMessage_C"))
                (set `/Game/Blueprints/UI/UI_Pickups/UI_GenericMessage.Message` (`KismetTextLibrary.Conv_StringToText` (`KismetStringLibrary.Concat_StrStr` (`KismetStringLibrary.Conv_IntToString` (+ (`self.Remaining time`) 1)) " minutes remaining")) _returnvalue)
                (`UserWidget.AddToViewport` _returnvalue 0)
                (`GameplayStatics.PlaySound2D` "/Game/AUDIO/SFX_UI/Alarms/AlertAlarm_04_Single.AlertAlarm_04_Single" 1.0 1.0 0.0 null null))))))
      (else
        (bind _output_get_3 (set `self.Value seconds` (- (`self.Value seconds`) 1)))
        (if (> _output_get_3 9)
          (set `/Game/Blueprints/UI/UI_Arcade/W_Timer.Seconds text` (`KismetTextLibrary.Conv_IntToText` _output_get_3) (`self.UI`))
          (else
            (set `/Game/Blueprints/UI/UI_Arcade/W_Timer.Seconds text` (`KismetTextLibrary.Conv_StringToText` (`KismetStringLibrary.Concat_StrStr` "0" (`KismetTextLibrary.Conv_TextToString` (`KismetTextLibrary.Conv_IntToText` _output_get_3)))) (`self.UI`))))))))

(fn `UserConstructionScript`)