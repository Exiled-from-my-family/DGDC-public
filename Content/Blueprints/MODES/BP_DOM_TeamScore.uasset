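; BP_DOM_TeamScore runs scoring for the Domination mode, tallying red and blue team points from control points.
; On BeginPlay it caches all BP_ControlPoint actors, then a looping timer adds a point per held point to its team.
; Reaching POINTSTOWIN declares the winner, removes the score widget and closes a gate against repeat declarations.
; Player respawn recreates the widget and replays the HUD's RedTeam animation after a short delay.
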(event `self.ReceiveBeginPlay`
  (bind _asfps_movement_character_light_1_vq_3 (cast `/Game/Blueprints/CHARACTERS/fpsMovementCharacter_light_1_vq3` (`GameplayStatics.GetPlayerPawn` 0)))
  (add `/Game/Blueprints/CHARACTERS/fpsMovementCharacter_light_1_vq3.respawned` _asfps_movement_character_light_1_vq_3 (delegate `redoscore`))
  (bind _returnvalue (`|CreateWidget` "/Game/Blueprints/UI/UI_Modes/UI_DOM_Score.UI_DOM_Score_C" (`GameplayStatics.GetPlayerController` 0)))
  (set `self.ui` _returnvalue)
  (`UserWidget.AddToViewport` _returnvalue 0)
  (`KismetSystemLibrary.K2_SetTimerDelegate` (delegate `score points`) 2.0 true)
  (bind _outactors (`GameplayStatics.GetAllActorsOfClass` "/Game/Blueprints/MODES/BP_ControlPoint.BP_ControlPoint_C"))
  (set `self.points` _outactors)
  (`KismetSystemLibrary.Delay` 0.02 :!label _label)
  (bind _hud (`/Game/Blueprints/CHARACTERS/fpsMovementCharacter_light_1_vq3.HUD` _asfps_movement_character_light_1_vq_3))
  (`UserWidget.PlayAnimation` _hud (`/Game/Blueprints/UI/HUD_vq3.RedTeam` _hud) 0.0 1 "Forward" 1.0 false))

(event `redoscore`
  (bind _returnvalue (`|CreateWidget` "/Game/Blueprints/UI/UI_Modes/UI_DOM_Score.UI_DOM_Score_C"))
  (set `self.ui` _returnvalue)
  (`UserWidget.AddToViewport` _returnvalue 0)
  (goto _label))

(event `score points`
  (bind _points (`self.points`))
  (for _index (range (`KismetArrayLibrary.Array_Length` _points))
    (bind _output (`|GetArrayItem` _points _index))
    (`/Engine/EditorBlueprintResources/StandardMacros.IsValid` _output
      (:`Is Valid`
        (bind _team (`/Game/Blueprints/MODES/BP_ControlPoint.Team` _output))
        (if (== _team "red")
          (set `self.TeamRed_Temp` (+ (`self.TeamRed_Temp`) 1))
          (elif (== _team "blue")
            (set `self.TeamBlue_Temp` (+ (`self.TeamBlue_Temp`) 1)))))))
  (`self.Score`))

(event `Score`
  (bind _points_to_win (`self.POINTS TO WIN`))
  (set `self.TeamRed_Score` (+ (`self.TeamRed_Score`) (`self.TeamRed_Temp`)))
  (set `self.TeamBlue_Score` (+ (`self.TeamBlue_Score`) (`self.TeamBlue_Temp`)))
  (set `self.TeamRed_Temp` 0)
  (set `self.TeamBlue_Temp` 0)
  (`/Engine/EditorBlueprintResources/StandardMacros.Gate` false :!label _label_2
    (:`Exit`
      (if (>= (`self.TeamRed_Score`) _points_to_win)
        (`self.WINNER DECLARED` true)
        (`Widget.RemoveFromParent` (`self.ui`) :!label _label_3)
        (goto _label_2 :!via `Close`)
        (elif (>= (`self.TeamBlue_Score`) _points_to_win)
          (`self.WINNER DECLARED` false)
          (goto _label_3))))))

(fn `UserConstructionScript`)