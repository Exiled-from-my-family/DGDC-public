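; Pickable BLUE flag for a capture-the-flag mode that can be taken by red bots or the player, or returned to base.
; A living blue bot's touch or the AutoRestoreBlue timeline's end unhides BP_Flag_Blue, clears Captured, announces the return and destroys this actor.
; A red or player pickup attaches a BP_FlagCarriable to the spine, sets Captured and stops the timeline.
; Pickups also switch red bots' behavior trees according to FlagCarrier.
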(event `self.ReceiveBeginPlay`
  ;[1 1 1] BLUE Flag returns visible after RED Team scores, BLUE Flag can be picked up again
  (`Timeline|auto restore blue` :!via `PlayFromStart` :!label _label
    (:`Finished`
      (bind _outactors (`GameplayStatics.GetAllActorsOfClass` "/Game/Blueprints/MODES/BP_Flag_Blue.BP_Flag_Blue_C" :!label _label_2))
      (for _array_element _outactors
        (`self.SetActorHiddenInGame` _array_element false)
        (`self.SetActorEnableCollision` true))
      (bind _returnvalue (`|CreateWidget` "/Game/Blueprints/UI/UI_Pickups/UI_Pickup_Flag.UI_Pickup_Flag_C"))
      (set `/Game/Blueprints/UI/UI_Pickups/UI_Pickup_Flag.Team` "BLUE Flag returned" _returnvalue)
      (`UserWidget.AddToViewport` _returnvalue 0)
      (bind _outactors_2 (`GameplayStatics.GetAllActorsOfClass` "/Game/Blueprints/MODES/BP_Flag_Blue.BP_Flag_Blue_C"))
      (set `/Game/Blueprints/MODES/BP_Flag_Blue.captured?` false (`|GetArrayItem` _outactors_2))
      (`GameplayStatics.PlaySound2D` "/Game/AUDIO/SFX_CTF/SC_FlagReturn.SC_FlagReturn" 2.0 1.0 0.0 null null)
      (`self.K2_DestroyActor`))))

(event `self.Capsule.OnComponentBeginOverlap`
  (params (OverlappedComponent :type "PrimitiveComponent Object Reference") (OtherActor :type "Actor Object Reference") (OtherComp :type "PrimitiveComponent Object Reference") (OtherBodyIndex :type Integer) (bFromSweep :type Boolean) (SweepResult :type "HitResult Structure (by ref)"))
  (bind _asep_2_blue (cast `/Game/MISSIONS/EP2/Characters/ep2_blue` OtherActor)
    (:`then`
      (if (not (`/Game/Blueprints/CHARACTERS/NoobotAI/Blueprints/AI_NoobotChar.IsDead?` _asep_2_blue))
        (`KismetSystemLibrary.Delay` 0.2)
        (goto _label_2)))
    (:`CastFailed`
      (bind _asep_2_red (cast `/Game/MISSIONS/EP2/Characters/ep2_red` OtherActor)
        (:`then`
          (if (not (`/Game/Blueprints/CHARACTERS/NoobotAI/Blueprints/AI_NoobotChar.IsDead?` _asep_2_red))
            (bind _returnvalue (`|CreateWidget` "/Game/Blueprints/UI/UI_Pickups/UI_GenericMessage.UI_GenericMessage_C"))
            (set `/Game/Blueprints/UI/UI_Pickups/UI_GenericMessage.Message` "A teammate has the BLUE flag!" _returnvalue)
            (`UserWidget.AddToViewport` _returnvalue 0)
            (`|ExecutionSequence`
              (:`then_0`
                ;[1 1 1] When a teammate carries the flag the others run a different behavior tree (Red TDM) 12/03/23 (to be implemented for Arcade bots in the future)
                (bind _outactors (`GameplayStatics.GetAllActorsOfClass` "/Game/MISSIONS/EP2/Characters/ep2_red.ep2_red_C"))
                (for _array_element _outactors
                  (if (`/Game/MISSIONS/EP2/Characters/ep2_red.flag carrier` _array_element)
                    (bind _returnvalue_2 (`AIBlueprintHelperLibrary.GetAIController` _array_element))
                    (`AIController.RunBehaviorTree` _returnvalue_2 "/Game/MISSIONS/EP3/Characters/red_cap_flag.red_cap_flag")
                    (else
                      (`AIController.RunBehaviorTree` _returnvalue_2 "/Game/MISSIONS/EP3/Characters/red_TDM.red_TDM")
                      (`KismetSystemLibrary.PrintString` "someone is already carrying the flag" true false)))))
              (:`then_1`
                (bind _returnvalue_3 (`|SpawnActorFromClass` "/Game/Blueprints/MODES/BP_FlagCarriable.BP_FlagCarriable_C" (`SceneComponent.GetSocketTransform` (`Character.Mesh` _asep_2_red) "spine_03" "RTS_World") "AlwaysSpawn" "OverrideRootScale" null false null))
                (`self.SetActorScale3D` _returnvalue_3 (0.75 0.75 0.75))
                (`self.K2_SetActorRotation` _returnvalue_3 (struct :`Pitch` 5.0 :`Yaw` 90.0 :`Roll` -20.0) false)
                (`self.K2_AttachToActor` _returnvalue_3 null "spine_03" "KeepWorld" "KeepRelative" "KeepRelative" true)
                (`self.K2_SetActorRelativeLocation` _returnvalue_3 (-70.0 0.0 60.0) false false)
                (`PrimitiveComponent.SetMaterial` (`/Game/Blueprints/MODES/BP_FlagCarriable.FlagMesh` _returnvalue_3) 0 "/Game/Blueprints/MODES/M_FlagNew.M_FlagNew")
                (`LightComponent.SetLightColor` (`/Game/Blueprints/MODES/BP_FlagCarriable.PointLight` _returnvalue_3) (struct :`R` 1.0 :`A` 1.0) true)
                (bind _outactors_2 (`GameplayStatics.GetAllActorsOfClass` "/Game/Blueprints/MODES/BP_Flag_Blue.BP_Flag_Blue_C" :!label _label_3))
                (set `/Game/Blueprints/MODES/BP_Flag_Blue.captured?` true (`|GetArrayItem` _outactors_2))
                (goto _label :!via `Stop`)))))
        (:`CastFailed`
          (bind _asfps_movement_character_light_1_vq_3 (cast `/Game/Blueprints/CHARACTERS/fpsMovementCharacter_light_1_vq3` OtherActor))
          (if (not (`/Game/Blueprints/CHARACTERS/fpsMovementCharacter_light_1_vq3.IsDead?` _asfps_movement_character_light_1_vq_3))
            (bind _returnvalue_4 (`|CreateWidget` "/Game/Blueprints/UI/UI_Pickups/UI_GenericMessage.UI_GenericMessage_C"))
            (set `/Game/Blueprints/UI/UI_Pickups/UI_GenericMessage.Message` "You got the BLUE flag!" _returnvalue_4)
            (`UserWidget.AddToViewport` _returnvalue_4 0)
            (`|ExecutionSequence`
              (:`then_0`
                (bind _returnvalue_5 (`|SpawnActorFromClass` "/Game/Blueprints/MODES/BP_FlagCarriable.BP_FlagCarriable_C" (`SceneComponent.GetSocketTransform` (`Character.Mesh` _asfps_movement_character_light_1_vq_3) "spine_03" "RTS_World") "AlwaysSpawn" "OverrideRootScale" null false null))
                (`self.SetActorScale3D` _returnvalue_5 (0.75 0.75 0.75))
                (`self.K2_SetActorRotation` _returnvalue_5 (struct :`Pitch` 5.0 :`Yaw` 90.0 :`Roll` -20.0) false)
                (`self.K2_AttachToActor` _returnvalue_5 null "spine_03" "KeepWorld" "KeepRelative" "KeepRelative" true)
                (`self.K2_SetActorRelativeLocation` _returnvalue_5 (-70.0 0.0 60.0) false false)
                (`PrimitiveComponent.SetMaterial` (`/Game/Blueprints/MODES/BP_FlagCarriable.FlagMesh` _returnvalue_5) 0 "/Game/Blueprints/MODES/M_FlagNew.M_FlagNew")
                (`LightComponent.SetLightColor` (`/Game/Blueprints/MODES/BP_FlagCarriable.PointLight` _returnvalue_5) (struct :`R` 1.0 :`A` 1.0) true)
                (goto _label_3))
              (:`then_1`
                (bind _outactors_3 (`GameplayStatics.GetAllActorsOfClass` "/Game/MISSIONS/EP2/Characters/ep2_red.ep2_red_C"))
                (for _array_element_2 _outactors_3
                  (if (not (`/Game/MISSIONS/EP2/Characters/ep2_red.flag carrier` _array_element_2))
                    (`AIController.RunBehaviorTree` (`AIBlueprintHelperLibrary.GetAIController` _array_element_2) "/Game/MISSIONS/EP3/Characters/red_TDM.red_TDM")
                    (`KismetSystemLibrary.PrintString` "someone is already carrying the flag" true false))))
              (:`then_2`
                (set `/Game/Blueprints/CHARACTERS/fpsMovementCharacter_light_1_vq3.FlagCarrier` true _asfps_movement_character_light_1_vq_3)))))))))

(fn `UserConstructionScript`
  (`PrimitiveComponent.CreateDynamicMaterialInstance` (`self.FlagMesh`) 0 null "None"))