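; Team Deathmatch score keeper that tallies red and blue kills and broadcasts the winner at a points limit.
; On BeginPlay it binds to death events of existing red and blue arcade bots, crediting the opposing team, and calls WINNERDECLARED with a red-win flag.
; It creates the score widget at start and again on player respawn, then plays the player HUD's RedTeam animation after a short delay.
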(event `self.ReceiveBeginPlay`
  (bind _asfps_movement_character_light_1_vq_3 (cast `/Game/Blueprints/CHARACTERS/fpsMovementCharacter_light_1_vq3` (`GameplayStatics.GetPlayerPawn` 0)))
  (add `/Game/Blueprints/CHARACTERS/fpsMovementCharacter_light_1_vq3.respawned` _asfps_movement_character_light_1_vq_3 (delegate `redoscore`))
  (bind _returnvalue (`|CreateWidget` "/Game/Blueprints/UI/UI_Modes/UI_TDM_Score.UI_TDM_Score_C" (`GameplayStatics.GetPlayerController` 0)))
  (set `self.UI` _returnvalue)
  (`UserWidget.AddToViewport` _returnvalue 10)
  (bind _outactors (`GameplayStatics.GetAllActorsOfClass` "/Game/MISSIONS/ARCADE/BOTS/BP_ArcadeBot_TeamRed.BP_ArcadeBot_TeamRed_C"))
  (for _array_element _outactors
    (add `/Game/MISSIONS/ARCADE/BOTS/BP_ArcadeBot_TeamRed.TeamRed_Dead` _array_element (delegate `blue scores`)))
  (bind _outactors_2 (`GameplayStatics.GetAllActorsOfClass` "/Game/MISSIONS/ARCADE/BOTS/BP_ArcadeBot_TeamBlue.BP_ArcadeBot_TeamBlue_C"))
  (for _array_element_2 _outactors_2
    (add `/Game/MISSIONS/ARCADE/BOTS/BP_ArcadeBot_TeamBlue.TeamBlue_Dead` _array_element_2 (delegate `red scores`)))
  (`KismetSystemLibrary.Delay` 0.02 :!label _label)
  (bind _hud (`/Game/Blueprints/CHARACTERS/fpsMovementCharacter_light_1_vq3.HUD` _asfps_movement_character_light_1_vq_3))
  (`UserWidget.PlayAnimation` _hud (`/Game/Blueprints/UI/HUD_vq3.RedTeam` _hud) 0.0 1 "Forward" 1.0 false))

(event `redoscore`
  (bind _returnvalue (`|CreateWidget` "/Game/Blueprints/UI/UI_Modes/UI_TDM_Score.UI_TDM_Score_C" (`GameplayStatics.GetPlayerController` 0)))
  (`UserWidget.AddToViewport` _returnvalue 0)
  (goto _label))

(event `red scores`
  (bind _result (`/Engine/EditorBlueprintResources/StandardMacros.IncrementInt` (`self.TeamRed_Score`))
    (:`  `
      (if (>= _result (`self.POINTS TO WIN`))
        (`self.WINNER DECLARED` true)))))

(event `blue scores`
  (`/Engine/EditorBlueprintResources/StandardMacros.IncrementInt` (`self.TeamBlue_Score`)
    (:`  `
      (if (>= (`self.TeamBlue_Score`) (`self.POINTS TO WIN`))
        (`self.WINNER DECLARED` false)))))

(fn `UserConstructionScript`)