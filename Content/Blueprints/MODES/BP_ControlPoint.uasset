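; Capturable team control point, apparently for a domination mode, with a rotating crystal, radius ring and world marker.
; While unlocked, a looping timer moves Status toward red for living players and red bots in the sphere, toward blue for blue bots.
; Reaching either limit or zero switches team visuals and sound; empty points drift back to their owner's limit, or zero if neutral.
; Player overlap shows a capture progress widget; captures fire team win dispatchers.
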(event `Worldmarker`
  (if (`self.Worldmarker?`)
    (bind _returnvalue (`|SpawnActorFromClass` "/Game/MISSIONS/EP0/Blueprints/BP_WorldMarker_Point.BP_WorldMarker_Point_C" (`self.GetTransform`) "Undefined" "OverrideRootScale" null null))
    (set `self.Widget` _returnvalue)))

(event `self.ReceiveBeginPlay`
  (`|ExecutionSequence`
    (:`then_0`
      (`KismetSystemLibrary.K2_SetTimerDelegate` (delegate `CheckIfLocked`) 0.03 true))
    (:`then_1`
      (`self.Worldmarker`))))

(event `Player respawn`
  (`SceneComponent.SetVisibility` (`/Game/MISSIONS/EP0/Blueprints/BP_WorldMarker_Point.DefaultSceneRoot` (`self.Widget`)) true true))

(event `CheckIfLocked`
  (bind _radius_ring (`self.Radius_Ring`))
  (bind _controlpoint (`self.ControlPoint`))
  (bind _radius_ring_2 (`self.Radius_Ring`))
  (bind _controlpoint_2 (`self.ControlPoint`))
  (bind _controlpoint_3 (`self.ControlPoint`))
  (bind _radius_ring_3 (`self.Radius_Ring`))
  (bind _status (`self.status`))
  (bind _team (`self.Team`))
  (bind _status_2 (`self.status`))
  (bind _status_3 (`self.status`))
  (bind _status_4 (`self.status`))
  (bind _returnvalue (== _status_4 -100.0))
  (bind _returnvalue_2 (== _status 100.0))
  (bind _overlappingactors (`PrimitiveComponent.GetOverlappingActors` (`self.Sphere`) "/Script/Engine.Character"))
  ;[1 1 1] set texts to tell which team is controlling the point and if it's unlocked
  (`TextRenderComponent.K2_SetText` (`self.TextRender`) (`KismetTextLibrary.Conv_StringToText` (`KismetStringLibrary.Concat_StrStr` (`KismetStringLibrary.Conv_NameToString` (`self.Team`)) " | " (`KismetStringLibrary.Conv_BoolToString` (`self.isUnlocked?`)))))
  ;[1 1 1] check if point is unlocked
  (if (`self.isUnlocked?`)
    (for _array_element _overlappingactors
      (`/Engine/EditorBlueprintResources/StandardMacros.IsValid` _array_element
        (:`Is Valid`
          (bind _asfps_movement_character_light_1_vq_3 (cast `/Game/Blueprints/CHARACTERS/fpsMovementCharacter_light_1_vq3` _array_element)
            (:`then`
              ;[1 1 1] charges the control point
              (if (not (or (`/Game/Blueprints/CHARACTERS/fpsMovementCharacter_light_1_vq3.IsDead?` _asfps_movement_character_light_1_vq_3) _returnvalue_2))
                (set `self.status` (+ (`self.capturespeed`) _status) :!label _label)
                ;[1 1 1] check status (100 for red team, -100 for blue)
                (if (== _status_3 0.0) :!label _label_2
                  ;[1 1 1] check status (returns to non when value goes to 0)
                  (if (not (== _team "None"))
                    (set `self.Team` "None")
                    ;[1 1 1] NONE
                    (`StaticMeshComponent.SetStaticMesh` _controlpoint "/Game/Blueprints/MODES/SM_ControlPoint_Neutral.SM_ControlPoint_Neutral")
                    (`PrimitiveComponent.SetMaterial` _controlpoint 0 "/Game/MATERIALS/M_Crystal.M_Crystal")
                    (`MeshComponent.SetVectorParameterValueOnMaterials` _radius_ring "Color" (1.0 1.0 1.0))
                    (`MeshComponent.SetScalarParameterValueOnMaterials` _radius_ring "Emissive" 24.0)
                    (`MeshComponent.SetScalarParameterValueOnMaterials` (`self.ControlPoint`) "Opacity" 0.4)
                    (`GameplayStatics.PlaySoundAtLocation` "/Game/AUDIO/SFX_DOM/SW_Control_TeamRed.SW_Control_TeamRed" (`SceneComponent.K2_GetComponentLocation` (`self.DefaultSceneRoot`)) (struct) 0.0 1.0 0.0 null null null)
                    (`LightComponent.SetLightColor` (`self.PointLight`) (struct :`R` 1.0 :`G` 1.0 :`B` 1.0 :`A` 1.0) true)
                    (`/Game/MISSIONS/EP0/Blueprints/BP_WorldMarker_Point.Team_NONE` (`self.Widget`)))
                  (elif (== _status_3 100.0)
                    (if (not (== _team "red"))
                      (set `self.Team` "red")
                      ;[1 0 0] RED
                      (`StaticMeshComponent.SetStaticMesh` _controlpoint_2 "/Game/Blueprints/MODES/SM_ControlPoint_Red.SM_ControlPoint_Red")
                      (`PrimitiveComponent.SetMaterial` _controlpoint_2 0 "/Game/MATERIALS/M_Crystal1.M_Crystal1")
                      (`MeshComponent.SetVectorParameterValueOnMaterials` _radius_ring_2 "Color" (1.0 0.05 0.0))
                      (`MeshComponent.SetScalarParameterValueOnMaterials` _radius_ring_2 "Emissive" 24.0)
                      (`MeshComponent.SetScalarParameterValueOnMaterials` (`self.ControlPoint`) "Opacity" 0.2)
                      (`GameplayStatics.PlaySoundAtLocation` "/Game/AUDIO/SFX_DOM/SC_ControlPoint_TeamRed.SC_ControlPoint_TeamRed" (`SceneComponent.K2_GetComponentLocation` (`self.DefaultSceneRoot`)) (struct) 1.0 1.0 0.0 null null null)
                      (`LightComponent.SetLightColor` (`self.PointLight`) (struct :`R` 1.0 :`G` 0.099899 :`A` 1.0) true)
                      (`self.red win` self)
                      (`/Game/MISSIONS/EP0/Blueprints/BP_WorldMarker_Point.Team_RED` (`self.Widget`))
                      (`KismetSystemLibrary.Delay` 1.0)
                      (`self.destroy_cap`))
                    (elif (== _status_3 -100.0)
                      (if (not (== _team "blue"))
                        ;[0 0.1228 1] BLUE
                        (set `self.Team` "blue")
                        (`StaticMeshComponent.SetStaticMesh` _controlpoint_3 "/Game/Blueprints/MODES/SM_ControlPoint_Blue.SM_ControlPoint_Blue")
                        (`PrimitiveComponent.SetMaterial` _controlpoint_3 0 "/Game/MATERIALS/M_Crystal2.M_Crystal2")
                        (`MeshComponent.SetVectorParameterValueOnMaterials` _radius_ring_3 "Color" (0.0 0.05 1.0))
                        (`MeshComponent.SetScalarParameterValueOnMaterials` _radius_ring_3 "Emissive" 24.0)
                        (`MeshComponent.SetScalarParameterValueOnMaterials` (`self.ControlPoint`) "Opacity" 0.2)
                        (`GameplayStatics.PlaySoundAtLocation` "/Game/AUDIO/SFX_DOM/SC_ControlPoint_TeamBlue.SC_ControlPoint_TeamBlue" (`SceneComponent.K2_GetComponentLocation` (`self.DefaultSceneRoot`)) (struct) 1.0 1.0 0.0 null null null)
                        (`LightComponent.SetLightColor` (`self.PointLight`) (struct :`G` 0.099899 :`B` 1.0 :`A` 1.0) true)
                        (`self.blue win` self)
                        (`/Game/MISSIONS/EP0/Blueprints/BP_WorldMarker_Point.Team_BLUE` (`self.Widget`))))))))
            (:`CastFailed`
              ;[1 0 0] Red bots
              (bind _asep_2_red (cast `/Game/MISSIONS/EP2/Characters/ep2_red` _array_element)
                (:`then`
                  (if (not (or _returnvalue_2 (`/Game/Blueprints/CHARACTERS/NoobotAI/Blueprints/AI_NoobotChar.IsDead?` _asep_2_red)))
                    (goto _label)))
                (:`CastFailed`
                  (bind _asbp_arcade_bot_team_red (cast `/Game/MISSIONS/ARCADE/BOTS/BP_ArcadeBot_TeamRed` _array_element)
                    (:`then`
                      (if (not (or _returnvalue_2 (`/Game/Blueprints/CHARACTERS/NoobotAI/Blueprints/AI_NoobotChar.IsDead?` _asbp_arcade_bot_team_red)))
                        (goto _label)))
                    (:`CastFailed`
                      ;[0 0.4588 1] Blue bots
                      (bind _asep_2_blue (cast `/Game/MISSIONS/EP2/Characters/ep2_blue` _array_element)
                        (:`then`
                          (if (not (or (`/Game/Blueprints/CHARACTERS/NoobotAI/Blueprints/AI_NoobotChar.IsDead?` _asep_2_blue) _returnvalue))
                            (set `self.status` (- _status_4 (`self.capturespeed`)) :!label _label_3)
                            (goto _label_2)))
                        (:`CastFailed`
                          (bind _asbp_arcade_bot_team_blue (cast `/Game/MISSIONS/ARCADE/BOTS/BP_ArcadeBot_TeamBlue` _array_element))
                          (if (not (or (`/Game/Blueprints/CHARACTERS/NoobotAI/Blueprints/AI_NoobotChar.IsDead?` _asbp_arcade_bot_team_blue) _returnvalue))
                            (goto _label_3)))))))))))))
    ;[1 1 1] REVERT CAPTURE
    (if (not (or (== _status_2 100.0) (== _status_2 -100.0) (`KismetMathLibrary.Conv_IntToBool` (`KismetArrayLibrary.Array_Length` _overlappingactors)) (== _status_2 0.0)))
      (set `self.status` (+ (* (`self.capturespeed`) (`KismetMathLibrary.SelectFloat` 1.0 -1.0 (< _status_2 0.0)) (`KismetMathLibrary.SelectFloat` 1.0 -1.0 (== (`self.Team`) "None"))) (`self.status`)))
      (goto _label_2))))

(event `self.ReceiveTick`
  (params (DeltaSeconds :type "Float (single-precision)"))
  ;[0.4315 1 0.9758 1 24] control point rotator
  (`SceneComponent.K2_AddLocalRotation` (`self.ControlPoint`) (`KismetMathLibrary.MakeRotator` 0.0 0.0 (* DeltaSeconds 20.0)) false false))

(event `self.Sphere.OnComponentBeginOverlap`
  (params (OverlappedComponent :type "PrimitiveComponent Object Reference") (OtherActor :type "Actor Object Reference") (OtherComp :type "PrimitiveComponent Object Reference") (OtherBodyIndex :type Integer) (bFromSweep :type Boolean) (SweepResult :type "HitResult Structure (by ref)"))
  (if (not (and (== (`self.status`) 100.0) (== (`self.Team`) "red")))
    (cast `/Game/Blueprints/CHARACTERS/fpsMovementCharacter_light_1_vq3` OtherActor)
    (bind _returnvalue (`|CreateWidget` "/Game/Blueprints/UI/UI_Modes/UI_DOM_CaptureProgress.UI_DOM_CaptureProgress_C"))
    (set `/Game/Blueprints/UI/UI_Modes/UI_DOM_CaptureProgress.point` self _returnvalue)
    (`UserWidget.AddToViewport` _returnvalue 0)))

(event `self.Sphere.OnComponentEndOverlap`
  (params (OverlappedComponent :type "PrimitiveComponent Object Reference") (OtherActor :type "Actor Object Reference") (OtherComp :type "PrimitiveComponent Object Reference") (OtherBodyIndex :type Integer))
  (cast `/Game/Blueprints/CHARACTERS/fpsMovementCharacter_light_1_vq3` OtherActor)
  (`self.destroy_cap`))

(fn `UserConstructionScript`
  (bind _controlpoint (`self.ControlPoint`))
  (`StaticMeshComponent.SetStaticMesh` _controlpoint "/Game/Blueprints/MODES/SM_ControlPoint_Neutral.SM_ControlPoint_Neutral")
  (`PrimitiveComponent.CreateDynamicMaterialInstance` _controlpoint 0 "/Game/MATERIALS/M_Crystal.M_Crystal" "None")
  (`PrimitiveComponent.CreateDynamicMaterialInstance` (`self.Radius_Ring`) 0 "/Game/Blueprints/PICKUPS/M_ControlPointRadius.M_ControlPointRadius" "None")
  (`MeshComponent.SetScalarParameterValueOnMaterials` (`self.ControlPoint`) "Opacity" 0.2)
  (`LightComponent.SetLightColor` (`self.PointLight`) (struct :`R` 1.0 :`G` 1.0 :`B` 1.0 :`A` 1.0) true))