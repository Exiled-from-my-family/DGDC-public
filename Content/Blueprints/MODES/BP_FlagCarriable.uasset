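; Carriable red or blue capture-the-flag flag that characters and bots pick up, drop on death or return.
; Capsule overlap attaches it to an opposing character's spine or returns it for its own team, re-showing the base flag actors.
; Death events make a player's flag drop and start an auto-return timeline.
; Bot-carried flags are destroyed instead, with blue respawning as a pickable, working around unreliable detaching.
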(event `self.ReceiveTick`
  (params (DeltaSeconds :type "Float (single-precision)"))
  (bind _returnvalue (`self.GetOwner`))
  (`/Engine/EditorBlueprintResources/StandardMacros.IsValid` _returnvalue
    (:`Is Valid`
      (bind _asep_2_blue (cast `/Game/MISSIONS/EP2/Characters/ep2_blue` _returnvalue)
        (:`then`
          (if (`/Game/Blueprints/CHARACTERS/NoobotAI/Blueprints/AI_NoobotChar.IsDead?` _asep_2_blue)
            (set `self.currently carried` false :!label _label)))
        (:`CastFailed`
          (bind _asfps_movement_character_light_1_vq_3 (cast `/Game/Blueprints/CHARACTERS/fpsMovementCharacter_light_1_vq3` _returnvalue)
            (:`then`
              (if (`/Game/Blueprints/CHARACTERS/fpsMovementCharacter_light_1_vq3.IsDead?` _asfps_movement_character_light_1_vq_3)
                (goto _label)))
            (:`CastFailed`
              (bind _asep_1_character (cast `/Game/MISSIONS/EP1/Characters/ep1_character` _returnvalue))
              (if (`/Game/Blueprints/CHARACTERS/NoobotAI/Blueprints/AI_NoobotChar.IsDead?` _asep_1_character)
                (goto _label)))))))
    (:`Is Not Valid`
      (goto _label))))

(event `self.ReceiveBeginPlay`
  (bind _returnvalue (`self.GetOwner`))
  (bind _asep_2_blue (cast `/Game/MISSIONS/EP2/Characters/ep2_blue` _returnvalue)
    (:`then`
      (add `/Game/MISSIONS/EP1/Characters/ep1_character.owned` _asep_2_blue (delegate `red restore flag`)))
    (:`CastFailed`
      (bind _asfps_movement_character_light_1_vq_3 (cast `/Game/Blueprints/CHARACTERS/fpsMovementCharacter_light_1_vq3` _returnvalue)
        (:`then`
          (add `/Game/Blueprints/CHARACTERS/fpsMovementCharacter_light_1_vq3.Died` _asfps_movement_character_light_1_vq_3 (delegate `blue restore flag`)))
        (:`CastFailed`
          (bind _asep_1_character (cast `/Game/MISSIONS/EP1/Characters/ep1_character` _returnvalue))
          (add `/Game/MISSIONS/EP1/Characters/ep1_character.owned` _asep_1_character (delegate `blue restore flag`)))))))

(event `blue restore flag`
  (params (`killed ep1_char` :type "/Game/MISSIONS/EP1/Characters/ep1_character Object Reference"))
  (bind _returnvalue (`self.GetAttachParentActor`))
  (`|ExecutionSequence`
    (:`then_0`
      (bind _asfps_movement_character_light_1_vq_3 (cast `/Game/Blueprints/CHARACTERS/fpsMovementCharacter_light_1_vq3` _returnvalue)
        (:`then`
          (remove `/Game/Blueprints/CHARACTERS/fpsMovementCharacter_light_1_vq3.Died` _asfps_movement_character_light_1_vq_3 (delegate `blue restore flag`))
          (`PrimitiveComponent.SetOwnerNoSee` (`self.FlagMesh`) false)
          (bind _returnvalue_2 (`self.K2_GetActorLocation` _asfps_movement_character_light_1_vq_3))
          (`self.K2_SetActorLocation` _returnvalue_2)
          (`self.K2_DetachFromActor` "KeepWorld" "KeepWorld" "KeepWorld")
          (set `self.currently carried` false)
          (`self.SetActorScale3D` (1.0 1.0 1.0))
          (`self.K2_SetActorRotation` (struct))
          (`self.K2_SetActorRelativeLocation` _returnvalue_2)
          (`Timeline|auto restore blue` :!via `PlayFromStart` :!label _label_2
            (:`Finished`
              ;[1 1 1] Blue Flag returns visible after RED Team scores, Blue Flag can be picked up again
              (bind _outactors (`GameplayStatics.GetAllActorsOfClass` "/Game/Blueprints/MODES/BP_Flag_Blue.BP_Flag_Blue_C" :!label _label_3))
              (for _array_element _outactors
                (`self.SetActorHiddenInGame` _array_element false)
                (`self.SetActorEnableCollision` _array_element true)
                (set `/Game/Blueprints/MODES/BP_Flag_Blue.captured?` false _array_element))
              (bind _returnvalue_3 (`|CreateWidget` "/Game/Blueprints/UI/UI_Pickups/UI_Pickup_Flag.UI_Pickup_Flag_C"))
              (set `/Game/Blueprints/UI/UI_Pickups/UI_Pickup_Flag.Team` "BLUE Flag returned" _returnvalue_3)
              (`UserWidget.AddToViewport` _returnvalue_3 0)
              (`GameplayStatics.PlaySound2D` "/Game/AUDIO/SFX_CTF/SC_FlagReturn.SC_FlagReturn" 2.0 1.0 0.0 null null :!label _label_4)
              (`self.K2_DestroyActor`))))
        (:`CastFailed`
          (bind _asep_1_character (cast `/Game/MISSIONS/EP1/Characters/ep1_character` _returnvalue :!pinned true) ; cast failed to unbind causing a problem?
            (:`then`
              (remove `/Game/MISSIONS/EP1/Characters/ep1_character.owned` _asep_1_character (delegate `blue restore flag`)))
            (:`CastFailed`
              _))
          ;[1 1 1] NEW SOLUTION FOR RED BOTS
          (`self.K2_DestroyActor`)
          (`KismetSystemLibrary.PrintString` "just destroy the flag")
          (`|SpawnActorFromClass` "/Game/Blueprints/MODES/BP_FlagPickable_blue.BP_FlagPickable_blue_C" (`KismetMathLibrary.MakeTransform` (`self.K2_GetActorLocation`)) "Undefined" "OverrideRootScale" null null)
          (`KismetSystemLibrary.PrintString` "SPAWNPICKABLE BLUE"))))
    (:`then_1`
      (`PrimitiveComponent.SetCollisionEnabled` (`self.Capsule`) "NoCollision")
      (`KismetSystemLibrary.Delay` 0.5)
      (`PrimitiveComponent.SetCollisionEnabled` (`self.Capsule`) "QueryOnly"))))

(event `red restore flag`
  (params (`killed ep1_char` :type "/Game/MISSIONS/EP1/Characters/ep1_character Object Reference"))
  (bind _asep_2_blue (cast `/Game/MISSIONS/EP2/Characters/ep2_blue` (`self.GetAttachParentActor`) :!pinned true) ; cast failed to unbind causing a problem?
    (:`then`
      (remove `/Game/MISSIONS/EP1/Characters/ep1_character.owned` _asep_2_blue (delegate `red restore flag`)))
    (:`CastFailed`
      _))
  ;[1 1 1] new solution
  (`self.K2_DestroyActor`))

(event `detach red flag from blue bot`
  ;[1 1 1] Flag_Carriable doesn't get detached from blue bot on death: instead it gets destroyed and a new one gets spanwed at location - this should solve the issue of the flag not detaching correctly from time to time
  (`KismetSystemLibrary.PrintString` "RED FLAG DETACH" true false)
  (bind _returnvalue (`|SpawnActorFromClass` "BP_FlagCarriable_C" (`KismetMathLibrary.MakeTransform` (`self.K2_GetActorLocation` (stale `red restore flag` _asep_2_blue))) "Undefined" "OverrideRootScale" null false null))
  (set `/Game/Blueprints/MODES/BP_FlagCarriable.red` true _returnvalue)
  (`PrimitiveComponent.SetMaterial` (`/Game/Blueprints/MODES/BP_FlagCarriable.FlagMesh` _returnvalue) 0 "/Game/Blueprints/MODES/M_FlagNew.M_FlagNew")
  (`LightComponent.SetLightColor` (`/Game/Blueprints/MODES/BP_FlagCarriable.PointLight` _returnvalue) (struct :`R` 1.0 :`A` 1.0) true)
  (set `/Game/Blueprints/MODES/BP_FlagCarriable.currently carried` false _returnvalue)
  (`TimelineComponent.PlayFromStart` (`/Game/Blueprints/MODES/BP_FlagCarriable.auto restore red` _returnvalue)))

(event `self.Capsule.OnComponentBeginOverlap`
  (params (OverlappedComponent :type "PrimitiveComponent Object Reference") (OtherActor :type "Actor Object Reference") (OtherComp :type "PrimitiveComponent Object Reference") (OtherBodyIndex :type Integer) (bFromSweep :type Boolean) (SweepResult :type "HitResult Structure (by ref)"))
  (if (not (`self.currently carried`))
    (bind _asep_2_blue (cast `/Game/MISSIONS/EP2/Characters/ep2_blue` OtherActor)
      (:`then`
        (if (`self.red`)
          (if (not (`/Game/Blueprints/CHARACTERS/NoobotAI/Blueprints/AI_NoobotChar.IsDead?` _asep_2_blue))
            (`GameplayStatics.PlaySound2D` "/Game/AUDIO/SFX_CTF/SC_FlagPickup_Enemy.SC_FlagPickup_Enemy" 1.0 1.0 0.0 null null)
            (bind _returnvalue (`|CreateWidget` "/Game/Blueprints/UI/UI_Pickups/UI_Pickup_Flag.UI_Pickup_Flag_C"))
            (set `/Game/Blueprints/UI/UI_Pickups/UI_Pickup_Flag.Team` "The enemy has your flag!" _returnvalue)
            (`UserWidget.AddToViewport` _returnvalue 0)
            (bind _player (`/Game/Blueprints/NewFunctionLibrary.get player` :!label _label_5))
            (remove `/Game/Blueprints/CHARACTERS/fpsMovementCharacter_light_1_vq3.Died` _player (delegate `blue restore flag`))
            (`self.SetActorScale3D` (0.75 0.75 0.75) :!label _label_6)
            (`self.K2_SetActorRotation` (struct :`Pitch` 5.0 :`Yaw` 90.0 :`Roll` -20.0))
            (`self.K2_AttachToActor` OtherActor "spine_03" "KeepWorld" "KeepRelative" "KeepRelative" false)
            (`self.K2_SetActorRelativeLocation` (-70.0 0.0 60.0))
            (set `self.currently carried` true)
            (`|ExecutionSequence`
              (:`then_0`
                (goto _label_2 :!via `Stop`))
              (:`then_1`
                (`Timeline|auto restore red` :!via `Stop`
                  (:`Finished`
                    ;[1 1 1] Red Flag returns visible after BLUE Team scores, Red Flag can be picked up again
                    (bind _outactors (`GameplayStatics.GetAllActorsOfClass` "/Game/Blueprints/MODES/BP_Flag_Red.BP_Flag_Red_C" :!label _label_7))
                    (for _array_element _outactors
                      (`self.SetActorHiddenInGame` _array_element false)
                      (`self.SetActorEnableCollision` _array_element true)
                      (set `/Game/Blueprints/MODES/BP_Flag_Red.Captured?` false _array_element))
                    (bind _returnvalue_2 (`|CreateWidget` "/Game/Blueprints/UI/UI_Pickups/UI_Pickup_Flag.UI_Pickup_Flag_C"))
                    (set `/Game/Blueprints/UI/UI_Pickups/UI_Pickup_Flag.Team` "RED Flag returned" _returnvalue_2)
                    (`UserWidget.AddToViewport` _returnvalue_2 0)
                    (goto _label_4))))))
          (else
            (`KismetSystemLibrary.Delay` 0.1)
            (goto _label_3))))
      (:`CastFailed`
        (bind _asep_2_red (cast `/Game/MISSIONS/EP2/Characters/ep2_red` OtherActor)
          (:`then`
            (if (`self.red`)
              (`KismetSystemLibrary.Delay` 0.1 :!label _label_8)
              (goto _label_7)
              (elif (not (`/Game/Blueprints/CHARACTERS/NoobotAI/Blueprints/AI_NoobotChar.IsDead?` _asep_2_red))
                (`GameplayStatics.PlaySound2D` "/Game/AUDIO/SFX_CTF/SC_FlagPickup.SC_FlagPickup" 1.0 1.0 0.0 null null)
                (bind _returnvalue_3 (`|CreateWidget` "/Game/Blueprints/UI/UI_Pickups/UI_GenericMessage.UI_GenericMessage_C"))
                (set `/Game/Blueprints/UI/UI_Pickups/UI_GenericMessage.Message` "A teammate has the BLUE flag!" _returnvalue_3)
                (`UserWidget.AddToViewport` _returnvalue_3 0)
                (goto _label_5))))
          (:`CastFailed`
            (bind _asfps_movement_character_light_1_vq_3 (cast `/Game/Blueprints/CHARACTERS/fpsMovementCharacter_light_1_vq3` OtherActor))
            (if (`self.red`)
              (goto _label_8)
              (elif (not (`/Game/Blueprints/CHARACTERS/fpsMovementCharacter_light_1_vq3.IsDead?` _asfps_movement_character_light_1_vq_3))
                (bind _returnvalue_4 (`|CreateWidget` "/Game/Blueprints/UI/UI_Pickups/UI_GenericMessage.UI_GenericMessage_C"))
                (set `/Game/Blueprints/UI/UI_Pickups/UI_GenericMessage.Message` "You got the BLUE flag!" _returnvalue_4)
                (`UserWidget.AddToViewport` _returnvalue_4 0)
                (add `/Game/Blueprints/CHARACTERS/fpsMovementCharacter_light_1_vq3.Died` _asfps_movement_character_light_1_vq_3 (delegate `blue restore flag`))
                (goto _label_6)))))))))

(fn `UserConstructionScript`
  (`PrimitiveComponent.CreateDynamicMaterialInstance` (`self.FlagMesh`) 0 null "None"))