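; BP_BossHealthbar is an actor that shows a named health bar widget for one of four episode bosses, chosen by the SwitchOnBoss integer.
; On BeginPlay it creates UI_BossHealthbar with the boss name and binds to the player character's respawn event.
; On respawn it creates a new widget, finds the matching boss actor by class and sets both main and catch-up bars from health over a hardcoded maximum.
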(event `self.ReceiveBeginPlay`
  (set `self.Boss Name` (select `int` (`self.SwitchOnBoss`) :`0` "Hacker" :`1` "K-Frame" :`2` "Helsing" :`3` "Galactamax CEO" :!type "Text"))
  (bind _asfps_movement_character_light_1_vq_3 (cast `/Game/Blueprints/CHARACTERS/fpsMovementCharacter_light_1_vq3` (`GameplayStatics.GetPlayerPawn` 0)))
  (add `/Game/Blueprints/CHARACTERS/fpsMovementCharacter_light_1_vq3.respawned` _asfps_movement_character_light_1_vq_3 (delegate `redoscore`))
  (bind _returnvalue (`|CreateWidget` "/Game/UI_BossHealthbar.UI_BossHealthbar_C" (`GameplayStatics.GetPlayerController` 0)))
  (set `/Game/UI_BossHealthbar.Boss_Name` (`self.Boss Name`) _returnvalue)
  (`UserWidget.AddToViewport` _returnvalue 0)
  (set `self.UI` _returnvalue))

(event `redoscore`
  (bind _returnvalue (`|CreateWidget` "/Game/UI_BossHealthbar.UI_BossHealthbar_C" (`GameplayStatics.GetPlayerController` 0)))
  (`UserWidget.AddToViewport` _returnvalue 0)
  (set `/Game/UI_BossHealthbar.Boss_Name` (`self.Boss Name`) _returnvalue)
  ;[1 1 1] heath update checks the HP of current boss managed via INT (hacker is 0, K-Frame is 1 etc.)
  (switch `int` (`self.SwitchOnBoss`)
    (:`0`
      (bind _outactors (`GameplayStatics.GetAllActorsOfClass` "/Game/MISSIONS/EP2/Characters/ep2_blue_hacker_takes_over_rumble.ep2_blue_hacker_takes_over_rumble_C"))
      (for _array_element _outactors
        _)
      (bind _mainbar (`/Game/UI_BossHealthbar.MainBar` _returnvalue))
      (bind _returnvalue_2 (/ (`/Game/Blueprints/CHARACTERS/NoobotAI/Blueprints/AI_NoobotChar.Health` _array_element) 750.0))
      (`ProgressBar.SetPercent` _mainbar _returnvalue_2)
      (bind _catchupbar (`/Game/UI_BossHealthbar.CatchupBar` _returnvalue))
      (`ProgressBar.SetPercent` _catchupbar _returnvalue_2))
    (:`1`
      (bind _outactors_2 (`GameplayStatics.GetAllActorsOfClass` "/Game/MISSIONS/EP3/Characters/EP3_robot_big.EP3_robot_big_C"))
      (for _array_element_2 _outactors_2
        _)
      (bind _returnvalue_3 (/ (`/Game/Blueprints/CHARACTERS/NoobotAI/Blueprints/AI_NoobotChar.Health` _array_element_2) 1000.0))
      (`ProgressBar.SetPercent` _mainbar _returnvalue_3)
      (`ProgressBar.SetPercent` _catchupbar _returnvalue_3))
    (:`2`
      (bind _outactors_3 (`GameplayStatics.GetAllActorsOfClass` "/Game/MISSIONS/EP5/Characters/EP5_Helsing.EP5_Helsing_C"))
      (for _array_element_3 _outactors_3
        _)
      (bind _returnvalue_4 (/ (`/Game/Blueprints/CHARACTERS/NoobotAI/Blueprints/AI_NoobotChar.Health` _array_element_3) 1000.0))
      (`ProgressBar.SetPercent` _mainbar _returnvalue_4)
      (`ProgressBar.SetPercent` _catchupbar _returnvalue_4))
    (:`3`
      (bind _outactors_4 (`GameplayStatics.GetAllActorsOfClass` "/Game/MISSIONS/EP6/Characters/EP6_CEOMECHA_v2.EP6_CEOMECHA_v2_C"))
      (for _array_element_4 _outactors_4
        _)
      (bind _returnvalue_5 (/ (`/Game/Blueprints/CHARACTERS/NoobotAI/Blueprints/AI_NoobotChar.Health` _array_element_4) 2000.0))
      (`ProgressBar.SetPercent` _mainbar _returnvalue_5)
      (`ProgressBar.SetPercent` _catchupbar _returnvalue_5))))

(fn `UserConstructionScript`)