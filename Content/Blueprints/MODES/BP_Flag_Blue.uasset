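; Blue team's capture-the-flag base flag, which the player or red bots steal and where blue scores with the red flag.
; On pickup it hides itself and attaches a spawned BP_FlagCarriable to the carrier, switching other Ep2 red bots to Red_TDM.
; Tick and capsule overlap both detect a red carriable, destroy it and award blue the point.
; Scoring restores BP_Flag_Red, clears blue carrier flags and restarts Ep2 bots' cap-flag behavior trees.
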(event `self.ReceiveTick`
  (params (DeltaSeconds :type "Float (single-precision)"))
  (bind _asbp_flag_carriable (cast `/Game/Blueprints/MODES/BP_FlagCarriable` (`|GetArrayItem` (`PrimitiveComponent.GetOverlappingActors` (`self.Capsule`) "/Game/Blueprints/MODES/BP_FlagCarriable.BP_FlagCarriable_C"))))
  (if (`/Game/Blueprints/MODES/BP_FlagCarriable.red` _asbp_flag_carriable)
    (`self.K2_DestroyActor` _asbp_flag_carriable)
    (`/Game/Blueprints/NewFunctionLibrary.clean all message widgets` :!label _label)
    (bind _returnvalue (`|CreateWidget` "/Game/Blueprints/UI/UI_Pickups/UI_Pickup_Flag.UI_Pickup_Flag_C"))
    (set `/Game/Blueprints/UI/UI_Pickups/UI_Pickup_Flag.Team` "BLUE Team scores!" _returnvalue)
    (set `/Game/Blueprints/UI/UI_Pickups/UI_Pickup_Flag.Color` (struct :`G` 0.083116 :`B` 1.0 :`A` 1.0) _returnvalue)
    (`UserWidget.AddToViewport` _returnvalue 0)
    (`GameplayStatics.PlaySound2D` "/Game/AUDIO/SFX_CTF/SC_FlagScore_TeamBlue.SC_FlagScore_TeamBlue" 1.0 1.0 0.0 null null)
    (`self.blue scores`)
    ;[1 1 1] Red Flag returns visible after Red Team scores, Red Flag can be picked up again
    (bind _outactors (`GameplayStatics.GetAllActorsOfClass` "/Game/Blueprints/MODES/BP_Flag_Red.BP_Flag_Red_C"))
    (for _array_element _outactors
      (`self.SetActorHiddenInGame` _array_element false)
      (`self.SetActorEnableCollision` _array_element true)
      (set `/Game/Blueprints/MODES/BP_Flag_Red.Captured?` false _array_element))
    ;[1 1 1] After a point has been scored all team members run the "cap flag" BT again 12/03/23
    (bind _outactors_2 (`GameplayStatics.GetAllActorsOfClass` "/Game/MISSIONS/EP2/Characters/ep2_red.ep2_red_C"))
    (for _array_element_2 _outactors_2
      (`AIController.RunBehaviorTree` (`AIBlueprintHelperLibrary.GetAIController` _array_element_2) "/Game/MISSIONS/EP3/Characters/red_cap_flag.red_cap_flag")
      (`KismetSystemLibrary.PrintString` "red cap flag" true false (struct :`R` 1.0 :`G` 0.09159 :`A` 1.0)))
    ;[1 1 1] After a point has been scored all blue team members run the "cap flag" BT again 12/03/23
    (bind _outactors_3 (`GameplayStatics.GetAllActorsOfClass` "/Game/MISSIONS/EP2/Characters/ep2_blue.ep2_blue_C"))
    (for _array_element_3 _outactors_3
      (set `/Game/MISSIONS/EP2/Characters/ep2_blue.flag carrier` false _array_element_3)
      (`AIController.RunBehaviorTree` (`AIBlueprintHelperLibrary.GetAIController` _array_element_3) "/Game/MISSIONS/EP3/Characters/blue_cap_flag.blue_cap_flag")
      (`KismetSystemLibrary.PrintString` "blue cap flag" true false (struct :`G` 0.369272 :`B` 1.0 :`A` 1.0)))
    ;[1 1 1] no blue team member is the carrier
    (bind _outactors_4 (`GameplayStatics.GetAllActorsOfClass` "/Game/MISSIONS/ARCADE/BOTS/BP_ArcadeBot_TeamBlue.BP_ArcadeBot_TeamBlue_C"))
    (for _array_element_4 _outactors_4
      (set `/Game/MISSIONS/ARCADE/BOTS/BP_ArcadeBot_TeamBlue.carrier` false _array_element_4))))

(event `self.Capsule.OnComponentBeginOverlap`
  (params (OverlappedComponent :type "PrimitiveComponent Object Reference") (OtherActor :type "Actor Object Reference") (OtherComp :type "PrimitiveComponent Object Reference") (OtherBodyIndex :type Integer) (bFromSweep :type Boolean) (SweepResult :type "HitResult Structure (by ref)"))
  (`|ExecutionSequence`
    (:`then_0`
      (bind _asbp_flag_carriable (cast `/Game/Blueprints/MODES/BP_FlagCarriable` OtherActor))
      (if (`/Game/Blueprints/MODES/BP_FlagCarriable.red` _asbp_flag_carriable)
        (`self.K2_DestroyActor` _asbp_flag_carriable)
        (goto _label)))
    (:`then_1`
      (bind _asfps_movement_character_light_1_vq_3 (cast `/Game/Blueprints/CHARACTERS/fpsMovementCharacter_light_1_vq3` OtherActor)
        (:`then`
          (if (not (`/Game/Blueprints/CHARACTERS/fpsMovementCharacter_light_1_vq3.IsDead?` _asfps_movement_character_light_1_vq_3))
            (`|ExecutionSequence`
              (:`then_0`
                (`GameplayStatics.PlaySound2D` "/Game/AUDIO/SFX_CTF/SC_FlagPickup.SC_FlagPickup" 1.0 1.0 0.0 null null)
                (`/Game/Blueprints/NewFunctionLibrary.clean all message widgets`)
                (bind _returnvalue (`|CreateWidget` "/Game/Blueprints/UI/UI_Pickups/UI_GenericMessage.UI_GenericMessage_C"))
                (set `/Game/Blueprints/UI/UI_Pickups/UI_GenericMessage.Message` "You got the BLUE flag!" _returnvalue)
                (`UserWidget.AddToViewport` _returnvalue 0)
                (`self.SetActorHiddenInGame` true)
                (`self.SetActorEnableCollision` false)
                (set `self.captured?` true))
              (:`then_1`
                (bind _returnvalue_2 (`|SpawnActorFromClass` "/Game/Blueprints/MODES/BP_FlagCarriable.BP_FlagCarriable_C" (`SceneComponent.GetSocketTransform` (`/Game/Blueprints/CHARACTERS/fpsMovementCharacter_light_1_vq3.3PCharacterMesh` _asfps_movement_character_light_1_vq_3) "spine_03" "RTS_World") "AlwaysSpawn" "OverrideRootScale" _asfps_movement_character_light_1_vq_3 false null))
                (`self.SetActorScale3D` _returnvalue_2 (0.75 0.75 0.75))
                (`self.K2_SetActorRotation` _returnvalue_2 (struct :`Pitch` 5.0 :`Yaw` 90.0 :`Roll` -20.0) false)
                (`self.K2_AttachToActor` _returnvalue_2 _asfps_movement_character_light_1_vq_3 "spine_03" "KeepWorld" "KeepRelative" "KeepRelative" true)
                (`self.K2_SetActorRelativeLocation` _returnvalue_2 (-70.0 0.0 60.0) false false)
                (`PrimitiveComponent.SetMaterial` (`/Game/Blueprints/MODES/BP_FlagCarriable.FlagMesh` _returnvalue_2) 0 "/Game/Blueprints/MODES/M_FlagNew_Inst.M_FlagNew_Inst")
                (`LightComponent.SetLightColor` (`/Game/Blueprints/MODES/BP_FlagCarriable.PointLight` _returnvalue_2) (struct :`R` 0.1 :`B` 1.0 :`A` 1.0) true)
                (`PrimitiveComponent.SetOwnerNoSee` (`/Game/Blueprints/MODES/BP_FlagCarriable.FlagMesh` _returnvalue_2) true))
              (:`then_2`
                (set `/Game/Blueprints/CHARACTERS/fpsMovementCharacter_light_1_vq3.FlagCarrier` true _asfps_movement_character_light_1_vq_3)))))
        (:`CastFailed`
          (bind _asep_2_red (cast `/Game/MISSIONS/EP2/Characters/ep2_red` OtherActor)
            (:`then`
              (if (not (`/Game/Blueprints/CHARACTERS/NoobotAI/Blueprints/AI_NoobotChar.IsDead?` _asep_2_red))
                ;[1 1 1] The bot capping the flag is designated as carrier
                (set `/Game/MISSIONS/EP2/Characters/ep2_red.flag carrier` true _asep_2_red)
                (`KismetSystemLibrary.PrintString` "BOT IS CARRYING")
                (`|ExecutionSequence`
                  (:`then_0`
                    (`GameplayStatics.PlaySound2D` "/Game/AUDIO/SFX_CTF/SC_FlagPickup.SC_FlagPickup" 1.0 1.0 0.0 null null)
                    (bind _returnvalue_3 (`|CreateWidget` "/Game/Blueprints/UI/UI_Pickups/UI_GenericMessage.UI_GenericMessage_C"))
                    (set `/Game/Blueprints/UI/UI_Pickups/UI_GenericMessage.Message` "A teammate has the BLUE flag!" _returnvalue_3)
                    (`UserWidget.AddToViewport` _returnvalue_3 0)
                    (`self.SetActorHiddenInGame` true)
                    (`self.SetActorEnableCollision` false)
                    (set `self.captured?` true))
                  (:`then_1`
                    (bind _returnvalue_4 (`|SpawnActorFromClass` "/Game/Blueprints/MODES/BP_FlagCarriable.BP_FlagCarriable_C" (`SceneComponent.GetSocketTransform` (`Character.Mesh` _asep_2_red) "spine_03" "RTS_Actor") "AlwaysSpawn" "OverrideRootScale" _asep_2_red false null))
                    (`self.SetActorScale3D` _returnvalue_4 (0.75 0.75 0.75))
                    (`self.K2_SetActorRotation` _returnvalue_4 (struct :`Pitch` 5.0 :`Yaw` 90.0 :`Roll` -20.0) false)
                    (`self.K2_AttachToActor` _returnvalue_4 _asep_2_red "spine_03" "KeepWorld" "KeepRelative" "KeepRelative" true)
                    (`self.K2_SetActorRelativeLocation` _returnvalue_4 (-70.0 0.0 60.0) false false)
                    (`PrimitiveComponent.SetMaterial` (`/Game/Blueprints/MODES/BP_FlagCarriable.FlagMesh` _returnvalue_4) 0 "/Game/Blueprints/MODES/M_FlagNew_Inst.M_FlagNew_Inst")
                    (`LightComponent.SetLightColor` (`/Game/Blueprints/MODES/BP_FlagCarriable.PointLight` _returnvalue_4) (struct :`R` 0.1 :`B` 1.0 :`A` 1.0) true))
                  (:`then_2`
                    ;[1 1 1] When a teammate carries the flag the others run a different behavior tree (Red TDM) 12/03/23 (to be implemented for Arcade bots in the future)
                    (bind _outactors (`GameplayStatics.GetAllActorsOfClass` "/Game/MISSIONS/EP2/Characters/ep2_red.ep2_red_C"))
                    (for _array_element _outactors
                      (if (not (`/Game/MISSIONS/EP2/Characters/ep2_red.flag carrier` _array_element))
                        (`AIController.RunBehaviorTree` (`AIBlueprintHelperLibrary.GetAIController` _array_element) "/Game/MISSIONS/EP3/Characters/red_TDM.red_TDM")
                        (`KismetSystemLibrary.PrintString` "someone is already carrying the flag" true false)))))))
            (:`CastFailed`
              (bind _asbp_arcade_bot_team_red (cast `/Game/MISSIONS/ARCADE/BOTS/BP_ArcadeBot_TeamRed` OtherActor))
              (if (not (`/Game/Blueprints/CHARACTERS/NoobotAI/Blueprints/AI_NoobotChar.IsDead?` _asbp_arcade_bot_team_red))
                (`|ExecutionSequence`
                  (:`then_0`
                    (`GameplayStatics.PlaySound2D` "/Game/AUDIO/SFX_CTF/SC_FlagPickup.SC_FlagPickup" 1.0 1.0 0.0 null null)
                    (bind _returnvalue_5 (`|CreateWidget` "/Game/Blueprints/UI/UI_Pickups/UI_GenericMessage.UI_GenericMessage_C"))
                    (set `/Game/Blueprints/UI/UI_Pickups/UI_GenericMessage.Message` "A teammate has the BLUE flag!" _returnvalue_5)
                    (`UserWidget.AddToViewport` _returnvalue_5 0)
                    (`self.SetActorHiddenInGame` true)
                    (`self.SetActorEnableCollision` false)
                    (set `self.captured?` true))
                  (:`then_1`
                    (bind _returnvalue_6 (`|SpawnActorFromClass` "/Game/Blueprints/MODES/BP_FlagCarriable.BP_FlagCarriable_C" (`SceneComponent.GetSocketTransform` (`Character.Mesh` _asbp_arcade_bot_team_red) "spine_03" "RTS_Actor") "AlwaysSpawn" "OverrideRootScale" _asbp_arcade_bot_team_red false null))
                    (`self.SetActorScale3D` _returnvalue_6 (0.75 0.75 0.75))
                    (`self.K2_SetActorRotation` _returnvalue_6 (struct :`Pitch` 5.0 :`Yaw` 90.0 :`Roll` -20.0) false)
                    (`self.K2_AttachToActor` _returnvalue_6 _asbp_arcade_bot_team_red "spine_03" "KeepWorld" "KeepRelative" "KeepRelative" true)
                    (`self.K2_SetActorRelativeLocation` _returnvalue_6 (-70.0 0.0 60.0) false false)
                    (`PrimitiveComponent.SetMaterial` (`/Game/Blueprints/MODES/BP_FlagCarriable.FlagMesh` _returnvalue_6) 0 "/Game/Blueprints/MODES/M_FlagNew_Inst.M_FlagNew_Inst")
                    (`LightComponent.SetLightColor` (`/Game/Blueprints/MODES/BP_FlagCarriable.PointLight` _returnvalue_6) (struct :`R` 0.1 :`B` 1.0 :`A` 1.0) true))
                  (:`then_2`
                    (set `/Game/MISSIONS/ARCADE/BOTS/BP_ArcadeBot_TeamRed.carrier` true _asbp_arcade_bot_team_red)))))))))))

(fn `UserConstructionScript`)