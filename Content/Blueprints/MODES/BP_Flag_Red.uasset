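; Red team's flag in capture-the-flag: blue bots steal it, and red scores by bringing the blue flag to it.
; On blue bot overlap it hides, spawns an attached red BP_FlagCarriable and flags the carrier, switching other Ep2_blue bots to TDM behavior trees.
; An overlapping blue carriable, also polled on Tick, is destroyed to score, restoring the blue flag, clearing carrier states and rerunning Ep2 bots' cap-flag trees.
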(event `self.Capsule.OnComponentBeginOverlap`
  (params (OverlappedComponent :type "PrimitiveComponent Object Reference") (OtherActor :type "Actor Object Reference") (OtherComp :type "PrimitiveComponent Object Reference") (OtherBodyIndex :type Integer) (bFromSweep :type Boolean) (SweepResult :type "HitResult Structure (by ref)"))
  (`|ExecutionSequence`
    (:`then_0`
      (bind _asep_2_blue (cast `/Game/MISSIONS/EP2/Characters/ep2_blue` OtherActor)
        (:`then`
          (if (not (`/Game/Blueprints/CHARACTERS/NoobotAI/Blueprints/AI_NoobotChar.IsDead?` _asep_2_blue))
            ;[1 1 1] The bot capping the flag is designated as carrier
            (set `/Game/MISSIONS/EP2/Characters/ep2_blue.flag carrier` true _asep_2_blue)
            (`|ExecutionSequence`
              (:`then_0`
                (`GameplayStatics.PlaySound2D` "/Game/AUDIO/SFX_CTF/SC_FlagPickup_Enemy.SC_FlagPickup_Enemy" 1.0 1.0 0.0 null null)
                (bind _returnvalue (`|CreateWidget` "/Game/Blueprints/UI/UI_Pickups/UI_Pickup_Flag.UI_Pickup_Flag_C"))
                (set `/Game/Blueprints/UI/UI_Pickups/UI_Pickup_Flag.Team` "The enemy has your flag!" _returnvalue)
                (`UserWidget.AddToViewport` _returnvalue 0)
                (`self.SetActorHiddenInGame` true)
                (`self.SetActorEnableCollision` false)
                (set `self.Captured?` true))
              (:`then_1`
                (bind _returnvalue_2 (`|SpawnActorFromClass` "/Game/Blueprints/MODES/BP_FlagCarriable.BP_FlagCarriable_C" (`KismetMathLibrary.MakeTransform` (`self.K2_GetActorLocation` _asep_2_blue)) "AlwaysSpawn" "OverrideRootScale" _asep_2_blue true null))
                (`self.SetActorScale3D` _returnvalue_2 (0.75 0.75 0.75))
                (`self.K2_SetActorRotation` _returnvalue_2 (struct :`Pitch` 5.0 :`Yaw` 90.0 :`Roll` -20.0) false)
                (`self.K2_AttachToComponent` _returnvalue_2 (`/Game/MISSIONS/EP2/Characters/ep2_blue.flag_socket` _asep_2_blue) "None" "KeepWorld" "SnapToTarget" "KeepRelative" true)
                (`self.K2_SetActorRelativeLocation` _returnvalue_2 (-70.0 0.0 60.0) false false)
                (`PrimitiveComponent.SetMaterial` (`/Game/Blueprints/MODES/BP_FlagCarriable.FlagMesh` _returnvalue_2) 0 "/Game/Blueprints/MODES/M_FlagNew.M_FlagNew")
                (`LightComponent.SetLightColor` (`/Game/Blueprints/MODES/BP_FlagCarriable.PointLight` _returnvalue_2) (struct :`R` 1.0 :`A` 1.0) true))
              (:`then_2`
                ;[1 1 1] When a  blue teammate carries the flag the others run a different behavior tree (blue TDM) 12/03/23 (to be implemented for Arcade bots in the future)
                (bind _outactors (`GameplayStatics.GetAllActorsOfClass` "/Game/MISSIONS/EP2/Characters/ep2_blue.ep2_blue_C"))
                (for _array_element _outactors
                  (if (not (`/Game/MISSIONS/EP2/Characters/ep2_blue.flag carrier` _array_element))
                    (`AIController.RunBehaviorTree` (`AIBlueprintHelperLibrary.GetAIController` _array_element) "/Game/MISSIONS/EP3/Characters/blue_TDM.blue_TDM")))))))
        (:`CastFailed`
          (bind _asbp_arcade_bot_team_blue (cast `/Game/MISSIONS/ARCADE/BOTS/BP_ArcadeBot_TeamBlue` OtherActor))
          (if (not (`/Game/Blueprints/CHARACTERS/NoobotAI/Blueprints/AI_NoobotChar.IsDead?` _asbp_arcade_bot_team_blue))
            (`|ExecutionSequence`
              (:`then_0`
                (`GameplayStatics.PlaySound2D` "/Game/AUDIO/SFX_CTF/SC_FlagPickup_Enemy.SC_FlagPickup_Enemy" 1.0 1.0 0.0 null null)
                (bind _returnvalue_3 (`|CreateWidget` "/Game/Blueprints/UI/UI_Pickups/UI_Pickup_Flag.UI_Pickup_Flag_C"))
                (set `/Game/Blueprints/UI/UI_Pickups/UI_Pickup_Flag.Team` "The enemy has your flag!" _returnvalue_3)
                (`UserWidget.AddToViewport` _returnvalue_3 0)
                (`self.SetActorHiddenInGame` true)
                (`self.SetActorEnableCollision` false)
                (set `self.Captured?` true))
              (:`then_1`
                (bind _returnvalue_4 (`|SpawnActorFromClass` "/Game/Blueprints/MODES/BP_FlagCarriable.BP_FlagCarriable_C" (`SceneComponent.GetSocketTransform` (`Character.Mesh` _asbp_arcade_bot_team_blue) "spine_03" "RTS_World") "AlwaysSpawn" "OverrideRootScale" _asbp_arcade_bot_team_blue true null))
                (`self.SetActorScale3D` _returnvalue_4 (0.75 0.75 0.75))
                (`self.K2_SetActorRotation` _returnvalue_4 (struct :`Pitch` 5.0 :`Yaw` 90.0 :`Roll` -20.0) false)
                (`self.K2_AttachToActor` _returnvalue_4 _asbp_arcade_bot_team_blue "spine_03" "KeepWorld" "KeepRelative" "KeepRelative" true)
                (`self.K2_SetActorRelativeLocation` _returnvalue_4 (-70.0 0.0 60.0) false false)
                (`PrimitiveComponent.SetMaterial` (`/Game/Blueprints/MODES/BP_FlagCarriable.FlagMesh` _returnvalue_4) 0 "/Game/Blueprints/MODES/M_FlagNew.M_FlagNew")
                (`LightComponent.SetLightColor` (`/Game/Blueprints/MODES/BP_FlagCarriable.PointLight` _returnvalue_4) (struct :`R` 1.0 :`A` 1.0) true))
              (:`then_2`
                (set `/Game/MISSIONS/ARCADE/BOTS/BP_ArcadeBot_TeamBlue.carrier` true _asbp_arcade_bot_team_blue)))))))
    (:`then_1`
      (bind _asbp_flag_carriable (cast `/Game/Blueprints/MODES/BP_FlagCarriable` OtherActor))
      (if (not (`/Game/Blueprints/MODES/BP_FlagCarriable.red` _asbp_flag_carriable))
        (`self.K2_DestroyActor` _asbp_flag_carriable)
        (bind _returnvalue_5 (`|CreateWidget` "/Game/Blueprints/UI/UI_Pickups/UI_Pickup_Flag.UI_Pickup_Flag_C" :!label _label))
        (set `/Game/Blueprints/UI/UI_Pickups/UI_Pickup_Flag.Team` "RED Team scores!" _returnvalue_5)
        (set `/Game/Blueprints/UI/UI_Pickups/UI_Pickup_Flag.Color` (struct :`R` 1.0 :`A` 1.0) _returnvalue_5)
        (`UserWidget.AddToViewport` _returnvalue_5 0)
        (`GameplayStatics.PlaySound2D` "/Game/AUDIO/SFX_CTF/SC_FlagScore_TeamRed.SC_FlagScore_TeamRed" 1.0 1.0 0.0 null null)
        (`self.red scores`)
        ;[1 1 1] Blue Flag returns visible after blue Team scores, Blue Flag can be picked up again
        (bind _outactors_2 (`GameplayStatics.GetAllActorsOfClass` "/Game/Blueprints/MODES/BP_Flag_Blue.BP_Flag_Blue_C"))
        (for _array_element_2 _outactors_2
          (`self.SetActorHiddenInGame` _array_element_2 false)
          (`self.SetActorEnableCollision` _array_element_2 true)
          (set `/Game/Blueprints/MODES/BP_Flag_Blue.captured?` false _array_element_2))
        ;[1 1 1] After a point has been scored all team members run the "cap flag" BT again 12/03/23
        (bind _outactors_3 (`GameplayStatics.GetAllActorsOfClass` "/Game/MISSIONS/EP2/Characters/ep2_red.ep2_red_C"))
        (for _array_element_3 _outactors_3
          (set `/Game/MISSIONS/EP2/Characters/ep2_red.flag carrier` false _array_element_3)
          (`AIController.RunBehaviorTree` (`AIBlueprintHelperLibrary.GetAIController` _array_element_3) "/Game/MISSIONS/EP3/Characters/red_cap_flag.red_cap_flag")
          (`KismetSystemLibrary.PrintString` "red cap flag" true false (struct :`R` 1.0 :`G` 0.09159 :`A` 1.0)))
        ;[1 1 1] After a point has been scored all blue team members run the "cap flag" BT again 12/03/23
        (bind _outactors_4 (`GameplayStatics.GetAllActorsOfClass` "/Game/MISSIONS/EP2/Characters/ep2_blue.ep2_blue_C"))
        (for _array_element_4 _outactors_4
          (set `/Game/MISSIONS/EP2/Characters/ep2_blue.flag carrier` false _array_element_4)
          (`AIController.RunBehaviorTree` (`AIBlueprintHelperLibrary.GetAIController` _array_element_4) "/Game/MISSIONS/EP3/Characters/blue_cap_flag.blue_cap_flag")
          (`KismetSystemLibrary.PrintString` "blue cap flag" true false (struct :`G` 0.369272 :`B` 1.0 :`A` 1.0)))
        ;[1 1 1] no red team member is the carrier
        (bind _outactors_5 (`GameplayStatics.GetAllActorsOfClass` "/Game/MISSIONS/ARCADE/BOTS/BP_ArcadeBot_TeamRed.BP_ArcadeBot_TeamRed_C"))
        (for _array_element_5 _outactors_5
          (set `/Game/MISSIONS/ARCADE/BOTS/BP_ArcadeBot_TeamRed.carrier` false _array_element_5))))))

(event `self.ReceiveTick`
  (params (DeltaSeconds :type "Float (single-precision)"))
  (bind _asbp_flag_carriable (cast `/Game/Blueprints/MODES/BP_FlagCarriable` (`|GetArrayItem` (`PrimitiveComponent.GetOverlappingActors` (`self.Capsule`) "/Game/Blueprints/MODES/BP_FlagCarriable.BP_FlagCarriable_C"))))
  (if (not (`/Game/Blueprints/MODES/BP_FlagCarriable.red` _asbp_flag_carriable))
    (`self.K2_DestroyActor` _asbp_flag_carriable)
    (goto _label)))

(fn `UserConstructionScript`)