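; Behavior tree task that makes a Noobot AI pawn strafe left when that side is clear.
; Each tick sphere-traces far to the pawn's left on Visibility; without a hit, it adds leftward movement input scaled by MvmtScale.
; Both branches finish after a short random delay, always reporting failure, even after strafing.
; A difficulty gate for arcade and campaign modes is left disconnected and never runs.
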(event `self.ReceiveTickAI`
  (params (OwnerController :type "AIController Object Reference") (ControlledPawn :type "Pawn Object Reference") (DeltaSeconds :type "Float (single-precision)"))
  (bind _returnvalue (`Actor.GetActorRightVector` ControlledPawn))
  (bind _returnvalue_2 (`Actor.K2_GetActorLocation` ControlledPawn))
  (bind (_outhit _returnvalue_3) (`KismetSystemLibrary.SphereTraceSingle` _returnvalue_2 (+ _returnvalue_2 (* _returnvalue -1000.0)) 20.0 "TraceTypeQuery1" false (`|MakeArray` ControlledPawn :!type "Actor Object Reference")))
  (if _returnvalue_3
    (`KismetSystemLibrary.Delay` (`KismetMathLibrary.RandomFloatInRange` 0.0 0.5))
    (`self.FinishExecute` false)
    (else
      (`Pawn.AddMovementInput` ControlledPawn (* _returnvalue -1.0) (`self.mvmt scale`) false) ; old value: 0.7
      (`KismetSystemLibrary.Delay` (`KismetMathLibrary.RandomFloatInRange` 0.0 0.5))
      (`self.FinishExecute` false))))