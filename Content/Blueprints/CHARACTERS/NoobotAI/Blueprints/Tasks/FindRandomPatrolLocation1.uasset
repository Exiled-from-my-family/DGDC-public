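; Behavior tree task for NoobotAI that picks a random patrol location and writes it to the PatrolLocation blackboard key.
; It projects a point behind the pawn and, if that lies within MaxDistanceFromPlayer of the player, picks a reachable navmesh point around it.
; Otherwise it picks one around the player within a fixed radius, keeping patrols near the player.
; It finishes successfully on both branches, but never finishes if the pawn is invalid.
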(event `self.ReceiveExecuteAI`
  (params (OwnerController :type "AIController Object Reference") (ControlledPawn :type "Pawn Object Reference"))
  (bind _returnvalue (`Actor.K2_GetActorLocation` (`GameplayStatics.GetPlayerCharacter` 0)))
  (bind _returnvalue_2 (+ (`Actor.K2_GetActorLocation` ControlledPawn) (* (`Actor.GetActorForwardVector` ControlledPawn) (* (`self.Distance`) -1.0))))
  (`/Engine/EditorBlueprintResources/StandardMacros.IsValid` ControlledPawn
    (:`Is Valid`
      (if (< (`KismetMathLibrary.Vector_Distance` _returnvalue_2 _returnvalue) (`self.max distance from player`))
        (`BTFunctionLibrary.SetBlackboardValueAsVector` (`self.PatrolLocation`) (`NavigationSystemV1.K2_GetRandomReachablePointInRadius` _returnvalue_2 (`self.Radius`) null null))
        (`self.FinishExecute` true)
        (else
          (`BTFunctionLibrary.SetBlackboardValueAsVector` (`self.PatrolLocation`) (`NavigationSystemV1.K2_GetRandomReachablePointInRadius` _returnvalue 1000.0 null null))
          (`self.FinishExecute` true))))))