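; Behavior tree task that makes a Noobot AI pawn strafe along its right vector.
; Each tick it sphere-traces to the pawn's right on the Visibility channel and, if clear, adds movement input scaled by MvmtScale.
; Both outcomes finish as failed after a short random delay.
; Difficulty checks that would gate strafing are left disconnected, so they never run.
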(event `self.ReceiveTickAI`
  (params (OwnerController :type "AIController Object Reference") (ControlledPawn :type "Pawn Object Reference") (DeltaSeconds :type "Float (single-precision)"))
  (bind _returnvalue (`Actor.K2_GetActorLocation` ControlledPawn))
  (bind _returnvalue_2 (`Actor.GetActorRightVector` ControlledPawn))
  (bind (_outhit _returnvalue_3) (`KismetSystemLibrary.SphereTraceSingle` _returnvalue (+ _returnvalue (* _returnvalue_2 1000.0)) 20.0 "TraceTypeQuery1" false (`|MakeArray` ControlledPawn :!type "Actor Object Reference")))
  (if _returnvalue_3
    (`KismetSystemLibrary.Delay` (`KismetMathLibrary.RandomFloatInRange` 0.0 0.5))
    (`self.FinishExecute` false)
    (else
      (`Pawn.AddMovementInput` ControlledPawn (* _returnvalue_2 1.0) (`self.mvmt scale`) false)
      (`KismetSystemLibrary.Delay` (`KismetMathLibrary.RandomFloatInRange` 0.0 0.5))
      (`self.FinishExecute` false))))