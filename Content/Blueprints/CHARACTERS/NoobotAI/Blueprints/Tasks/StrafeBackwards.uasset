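; Behavior tree task that makes a Noobot AI pawn strafe backwards when the space behind it is clear.
; Each AI tick sphere-traces on Visibility behind the pawn, adding movement input only when nothing is hit.
; The input direction is a negated, scaled point ahead of the mesh, so it depends on world position rather than purely on facing.
; Both branches finish as failed after a short random delay.
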(event `self.ReceiveTickAI`
  (params (OwnerController :type "AIController Object Reference") (ControlledPawn :type "Pawn Object Reference") (DeltaSeconds :type "Float (single-precision)"))
  (bind _returnvalue (`Actor.K2_GetActorLocation` ControlledPawn))
  (bind (_outhit _returnvalue_2) (`KismetSystemLibrary.SphereTraceSingle` _returnvalue (+ _returnvalue (* (`Actor.GetActorForwardVector` ControlledPawn) -750.0)) 20.0 "TraceTypeQuery1" false (`|MakeArray` ControlledPawn :!type "Actor Object Reference") "None" true (struct :`R` 1.0 :`G` 0.739271 :`A` 1.0)))
  (if _returnvalue_2
    (`KismetSystemLibrary.Delay` (`KismetMathLibrary.RandomFloatInRange` 0.0 0.5))
    (`self.FinishExecute` false)
    (else
      (`Pawn.AddMovementInput` ControlledPawn (* (+ (`SceneComponent.K2_GetComponentLocation` (`|GetArrayItem` (`|MakeArray` (`Actor.GetComponentByClass` ControlledPawn "/Script/Engine.MeshComponent")))) (* (`Actor.GetActorForwardVector` ControlledPawn) 1500.0)) -0.75) 1.0 false)
      (`KismetSystemLibrary.Delay` (`KismetMathLibrary.RandomFloatInRange` 0.1 0.5))
      (`self.FinishExecute` false))))