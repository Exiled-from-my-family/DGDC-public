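; Behavior tree task for the Noobot AI that attempts a short forward move for the controlled pawn.
; Each tick sphere-traces ahead on the Visibility channel, ignoring the pawn.
; If clear, it adds movement input using mesh location plus a forward offset, a world position rather than a pure direction.
; Both branches finish as failed after a short random delay.
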(event `self.ReceiveTickAI`
  (params (OwnerController :type "AIController Object Reference") (ControlledPawn :type "Pawn Object Reference") (DeltaSeconds :type "Float (single-precision)"))
  (bind _returnvalue (`Actor.K2_GetActorLocation` ControlledPawn))
  (bind (_outhit _returnvalue_2) (`KismetSystemLibrary.SphereTraceSingle` _returnvalue (+ _returnvalue (* (`Actor.GetActorForwardVector` ControlledPawn) 1000.0)) 20.0 "TraceTypeQuery1" false (`|MakeArray` ControlledPawn :!type "Actor Object Reference")))
  (if _returnvalue_2
    (`KismetSystemLibrary.Delay` (`KismetMathLibrary.RandomFloatInRange` 0.0 0.5))
    (`self.FinishExecute` false)
    (else
      (`Pawn.AddMovementInput` ControlledPawn (* (+ (`SceneComponent.K2_GetComponentLocation` (`|GetArrayItem` (`|MakeArray` (`Actor.GetComponentByClass` ControlledPawn "/Script/Engine.MeshComponent")))) (* (`Actor.GetActorForwardVector` ControlledPawn) 750.0)) 1.0) 1.0 false)
      (`KismetSystemLibrary.Delay` (`KismetMathLibrary.RandomFloatInRange` 0.1 0.5))
      (`self.FinishExecute` false))))