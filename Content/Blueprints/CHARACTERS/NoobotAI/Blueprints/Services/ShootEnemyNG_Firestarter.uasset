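; Behavior tree service that lets the flamethrower security robot attack its blackboard enemy.
; Each tick tests a view cone, tight with a line-trace hit for Noobot targets, wider without requiring a hit for others.
; A living, visible target in range sets the nailgun blackboard flag and, after a wind-up, triggers a sound and delay-spaced burst of shoot messages.
; A dead non-Noobot target is cleared from the blackboard and the robot's state updates.
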(event `self.ReceiveTickAI`
  (params (OwnerController :type "AIController Object Reference") (ControlledPawn :type "Pawn Object Reference") (DeltaSeconds :type "Float (single-precision)"))
  (bind _array (`|MakeArray` "ObjectTypeQuery3" "ObjectTypeQuery1" "ObjectTypeQuery2" :!type "EObjectTypeQuery Enum"))
  (bind _enemy_ref (`self.Enemy_Ref`))
  (bind _currentrobot_ref (`self.CurrentRobot_Ref`))
  (bind _enemy_ref_2 (`self.Enemy_Ref`))
  (bind _enemy_ref_3 (`self.Enemy_Ref`))
  (bind _currentrobot_ref_2 (`self.CurrentRobot_Ref`))
  (bind _currentrobot_ref_3 (`self.CurrentRobot_Ref`))
  (bind _returnvalue (`BTFunctionLibrary.GetBlackboardValueAsActor` (`self.EnemyKey`)))
  (bind _array_2 (`|MakeArray` (`self.CurrentRobot_Ref`) :!type "Actor Object Reference"))
  (`/Engine/EditorBlueprintResources/StandardMacros.IsValid` ControlledPawn
    (:`Is Valid`
      (set `self.CurrentRobot_Ref` ControlledPawn)
      (`/Engine/EditorBlueprintResources/StandardMacros.IsValid` _returnvalue
        (:`Is Valid`
          (set `self.Enemy_Ref` _returnvalue)
          (bind _asai_noobot_char (cast `/Game/Blueprints/CHARACTERS/NoobotAI/Blueprints/AI_NoobotChar` ControlledPawn))
          (`|ExecutionSequence`
            (:`then_0`
              (bind _asai_noobot_char_2 (cast `/Game/Blueprints/CHARACTERS/NoobotAI/Blueprints/AI_NoobotChar` _enemy_ref)
                (:`then`
                  (bind _returnvalue_2 (message `/Game/Blueprints/CHARACTERS/NoobotAI/Blueprints/AI_Interface.GetShooterLocation` _currentrobot_ref))
                  (bind _returnvalue_3 (`Actor.K2_GetActorLocation` _asai_noobot_char_2))
                  (bind _outhit (`KismetSystemLibrary.LineTraceSingleForObjects` _returnvalue_2 _returnvalue_3 _array false _array_2))
                  (set `self.EnemyInSight` (and (== (`KismetMathLibrary.FindLookAtRotation` _returnvalue_2 _returnvalue_3) (`Actor.K2_GetActorRotation` _currentrobot_ref) :`ErrorTolerance` 25.0) (== _enemy_ref (`.HitActor` (`GameplayStatics.BreakHitResult` _outhit)))))
                  (set `/Game/Blueprints/CHARACTERS/NoobotAI/Blueprints/AI_NoobotChar.IsAtDistance` true _asai_noobot_char))
                (:`CastFailed`
                  (bind _returnvalue_4 (message `/Game/Blueprints/CHARACTERS/Character_Interface.GetHeadLocation` _enemy_ref))
                  (bind _returnvalue_5 (message `/Game/Blueprints/CHARACTERS/NoobotAI/Blueprints/AI_Interface.GetShooterLocation` _currentrobot_ref))
                  (bind _outhit_2 (`KismetSystemLibrary.LineTraceSingleForObjects` _returnvalue_5 _returnvalue_4 _array false _array_2))
                  (set `self.EnemyInSight` (and (!= (`GameplayStatics.GetObjectClass` _asai_noobot_char) "/Game/MISSIONS/EP2/Characters/ep2_red.ep2_red_C") (== (`KismetMathLibrary.FindLookAtRotation` _returnvalue_5 _returnvalue_4) (`Actor.K2_GetActorRotation` _currentrobot_ref_2) :`ErrorTolerance` 75.0)))
                  (set `/Game/Blueprints/CHARACTERS/NoobotAI/Blueprints/AI_NoobotChar.IsAtDistance` true _asai_noobot_char))))
            (:`then_1`
              (bind _asai_noobot_char_3 (cast `/Game/Blueprints/CHARACTERS/NoobotAI/Blueprints/AI_NoobotChar` _enemy_ref_2)
                (:`then`
                  (if (not (`/Game/Blueprints/CHARACTERS/NoobotAI/Blueprints/AI_NoobotChar.IsDead?` _asai_noobot_char_3))
                    (if (and (`self.EnemyInSight`) (< (`Actor.GetDistanceTo` (`self.CurrentRobot_Ref`) (`self.Enemy_Ref`)) (`self.Attack Distance`))) :!label _label
                      (`BTFunctionLibrary.SetBlackboardValueAsBool` (`self.RocketLauncherSelected`))
                      (`BTFunctionLibrary.SetBlackboardValueAsBool` (`self.NailgunSelected`) true)
                      (`KismetSystemLibrary.PrintString` "FIRESTARTER" true false (struct :`G` 0.66 :`B` 1.0 :`A` 1.0) 0.5)
                      (bind _asep4_security_flamethrower (cast `/Game/MISSIONS/EP4/Characters/EP4_Security_Flamethrower` ControlledPawn))
                      (if (not (`/Game/Blueprints/CHARACTERS/NoobotAI/Blueprints/AI_NoobotChar.IsDead?` _asep4_security_flamethrower))
                        (`KismetSystemLibrary.Delay` 2.0)
                        (set `/Game/Blueprints/CHARACTERS/NoobotAI/Blueprints/AI_NoobotChar.IsFiring?` true _asep4_security_flamethrower)
                        (`GameplayStatics.SpawnSoundAtLocation` "/Game/AUDIO/SFX_Weapons/Weap_ShockinTruth/SW_ElectroLaser_Activate.SW_ElectroLaser_Activate" (`Actor.K2_GetActorLocation` _asep4_security_flamethrower) (struct) 2.0 1.0 0.0 "/Game/kosm_fps_assets/Misc/SoundFX/SoundAttenuationGunShots.SoundAttenuationGunShots" null)
                        (message `/Game/Blueprints/CHARACTERS/NoobotAI/Blueprints/AI_Interface.ShootEnemyNew` _currentrobot_ref_3 _enemy_ref_3)
                        (`KismetSystemLibrary.Delay` (`self.Delay`))
                        (message `/Game/Blueprints/CHARACTERS/NoobotAI/Blueprints/AI_Interface.ShootEnemyNew` _currentrobot_ref_3 _enemy_ref_3)
                        (`KismetSystemLibrary.Delay` (`self.Delay`))
                        (message `/Game/Blueprints/CHARACTERS/NoobotAI/Blueprints/AI_Interface.ShootEnemyNew` _currentrobot_ref_3 _enemy_ref_3)
                        (`KismetSystemLibrary.Delay` (`self.Delay`))
                        (message `/Game/Blueprints/CHARACTERS/NoobotAI/Blueprints/AI_Interface.ShootEnemyNew` _currentrobot_ref_3 _enemy_ref_3)
                        (`KismetSystemLibrary.Delay` (`self.Delay`))
                        (message `/Game/Blueprints/CHARACTERS/NoobotAI/Blueprints/AI_Interface.ShootEnemyNew` _currentrobot_ref_3 _enemy_ref_3)
                        (`KismetSystemLibrary.Delay` (`self.Delay`))
                        (message `/Game/Blueprints/CHARACTERS/NoobotAI/Blueprints/AI_Interface.ShootEnemyNew` (`self.CurrentRobot_Ref`) (`self.Enemy_Ref`))
                        (`KismetSystemLibrary.Delay` (`self.Delay`))
                        (set `/Game/Blueprints/CHARACTERS/NoobotAI/Blueprints/AI_NoobotChar.IsFiring?` false _asep4_security_flamethrower)))))
                (:`CastFailed`
                  (bind _return_value (message `/Game/Blueprints/CHARACTERS/Character_Interface.IsAlive` _enemy_ref_2))
                  (if _return_value
                    (goto _label)
                    (else
                      (`BTFunctionLibrary.ClearBlackboardValue` (`self.EnemyKey`))
                      (message `/Game/Blueprints/CHARACTERS/NoobotAI/Blueprints/AI_Interface.UpdateState` _currentrobot_ref_2)
                      (`KismetSystemLibrary.PrintString` "dead"))))))))))))