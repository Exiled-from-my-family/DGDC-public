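; Noobot AI enemy character that takes damage, shows health feedback and ragdolls on death before being destroyed.
; Any damage splits between armor and health while armor remains, replicated through multicasts, updating a 3D health bar and spawning floating damage numbers with headshot styling.
; Death plays effects, disables hit collision and simulates physics from the pelvis, with an IsDead OnRep backup.
; Tick drives low-health and armor-break sounds and eases rotation upright after portals.
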(event `self.ReceiveTick`
  (params (DeltaSeconds :type "Float (single-precision)"))
  (bind _returnvalue (`self.K2_GetActorLocation`))
  ;[1 0.8067 0.3347] Event Tick
  (`|ExecutionSequence`
    (:`then_0`
      (if (<= (`self.Health`) 25.0)
        (`/Engine/EditorBlueprintResources/StandardMacros.DoOnce` false :!label _label
          (:`Completed`
            (`GameplayStatics.PlaySoundAtLocation` "/Game/AUDIO/SFX_Damage/low_health_2_Cue.low_health_2_Cue" _returnvalue (struct) 1.0 1.0 0.0 "/Game/kosm_fps_assets/Misc/SoundFX/SoundAttenuationNormal.SoundAttenuationNormal" null null)))
        (else
          (goto _label :!via `Reset`))))
    (:`then_1`
      (if (<= (`self.Armor`) 0.1)
        (`/Engine/EditorBlueprintResources/StandardMacros.DoOnce` false :!label _label_2
          (:`Completed`
            (`GameplayStatics.PlaySoundAtLocation` "/Game/AUDIO/SFX_Damage/SC_ArmorBreak.SC_ArmorBreak" _returnvalue (struct) 1.0 1.0 0.0 "/Game/kosm_fps_assets/Misc/SoundFX/SoundAttenuationNormal.SoundAttenuationNormal" null null)))
        (else
          (goto _label_2 :!via `Reset`))))
    (:`then_2`
      (`self.PortalRotationTracking`))))

(event `self.ReceiveAnyDamage`
  (params (Damage :type "Float (single-precision)") (DamageType :type "DamageType Object Reference") (InstigatedBy :type "Controller Object Reference") (DamageCauser :type "Actor Object Reference"))
  (bind _returnvalue (`self.K2_GetActorLocation`))
  (bind _mesh (`self.Mesh`))
  (bind _capsulecomponent (`self.CapsuleComponent`))
  ;[1 0 0] Damage
  ;;[1 1 1] On Any Damage
  (if (`.bSuccess` (cast `/Game/Blueprints/PROJECTILES/BP_Proj_ShockinTruth` DamageCauser :!pure true))
    (`KismetSystemLibrary.Delay` 0.03))
  (if (and (not (`self.IsDead?`)) (> (`self.Health`) 0.0))
    (`self.OnDamagePitchAudio` Damage)
    (if (> (`self.Armor`) 0.0)
      (`self.Armor > 0 Damage Multicast` Damage)
      (else
        (`self.HealthDamageMulticast` Damage)))
    (`/Engine/EditorBlueprintResources/StandardMacros.CompareFloat` (`self.Health`)
      (:`==`
        (set `self.IsDead?` true)
        (`GameplayStatics.SpawnEmitterAtLocation` null _returnvalue)
        (`|ExecutionSequence` :!label _label_3
          (:`then_0`
            (`GameplayStatics.PlaySoundAtLocation` "/Game/AUDIO/SFX_Damage/SC_FemaleDeath.SC_FemaleDeath" _returnvalue (struct) 1.0 1.0 0.0 null null null))
          (:`then_1`
            (`PrimitiveComponent.SetCollisionResponseToChannel` _capsulecomponent "ECC_GameTraceChannel1" "ECR_Ignore")
            (`PrimitiveComponent.SetCollisionResponseToChannel` (`self.Mesh`) "ECC_GameTraceChannel1" "ECR_Ignore")
            (`PrimitiveComponent.SetCollisionResponseToChannel` _capsulecomponent "ECC_Visibility" "ECR_Ignore")
            (`PrimitiveComponent.SetCollisionResponseToChannel` (`self.Mesh`) "ECC_Visibility" "ECR_Ignore")
            (`PrimitiveComponent.SetCollisionResponseToChannel` _capsulecomponent "ECC_Pawn" "ECR_Ignore")
            (`KismetSystemLibrary.Delay` 0.05)
            (`SkeletalMeshComponent.SetAllBodiesBelowSimulatePhysics` _mesh "pelvis" true true)
            (`SkeletalMeshComponent.SetAllBodiesBelowPhysicsBlendWeight` _mesh "pelvis" 1.0 false true)
            (`PrimitiveComponent.SetCollisionEnabled` _mesh "QueryAndPhysics")
            (`KismetSystemLibrary.Delay` 3.0)
            (`self.K2_DestroyActor`)))))))

(event `IsDeadMulticast`
  ;[1 0 0] Damage
  ;;[1 1 1] On Any Damage
  (goto _label_3))

(event `IsDeadServer`
  ;[1 0 0] Damage
  ;;[1 1 1] On Any Damage
  (`self.IsDeadMulticast`))

(event `HealthDamageMulticast`
  (params (Damage :type "Float (double-precision)"))
  ;[1 0 0] Damage
  ;;[1 1 1] Health Damage
  (set `self.Health` (`KismetMathLibrary.FClamp` (- (`self.Health`) Damage) 0.0 100.0))
  (message `/Game/Blueprints/UI/UI_Interface.SetHealthBarPercent` (`WidgetComponent.GetUserWidgetObject` (`self.HealthBar_3D_WG`)) (/ (`self.Health`) 100.0))
  (`/Engine/EditorBlueprintResources/ActorMacros.Switch Has Authority`
    (:`Authority`
      (`self.DisplayDamageServer` Damage (stale `self.ReceiveRadialDamage` HitInfo)))))

(event `DisplayDamageServer`
  (params (Damage :type "Float (double-precision)") (`Radial Hit Info` :type "HitResult Structure"))
  ;[1 0 0] Damage
  ;;[1 1 1] Health Damage
  (`self.DisplayDamage` Damage `Radial Hit Info`))

(event `OnLandedMulticast`
  ;[1 0 0] Damage
  ;;[1 1 1] On Landed
  (`GameplayStatics.PlaySoundAtLocation` "/Game/AUDIO/SFX_Movement/SC_Land.SC_Land" (`self.K2_GetActorLocation`) (struct) 0.5 1.0 0.0 null null null))

(event `self.OnLanded`
  (params (Hit :type "HitResult Structure (by ref)"))
  ;[1 0 0] Damage
  ;;[1 1 1] On Landed
  (`/Engine/EditorBlueprintResources/ActorMacros.Switch Has Authority`
    (:`Authority`
      (`self.OnLandedMulticast`))
    (:`Remote`
      (`self.OnLandedServer`))))

(event `HealthDamageClient`
  (params (Damage :type "Float (double-precision)"))
  ;[1 0 0] Damage
  ;;[1 1 1] Health Damage
  (`self.HealthDamageMulticast` Damage))

(event `Armor > 0 Damage Multicast`
  (params (ArmorDamage :type "Float (double-precision)"))
  (bind _returnvalue (/ ArmorDamage 2.0))
  ;[1 0 0] Damage
  ;;[1 1 1] Health Damage
  (set `self.Armor` (`KismetMathLibrary.FClamp` (- (`self.Armor`) (/ ArmorDamage 2.0)) 0.0 50.0))
  (message `/Game/Blueprints/UI/UI_Interface.SetArmorBarPercent` (`WidgetComponent.GetUserWidgetObject` (`self.HealthBar_3D_WG`)) (/ (`self.Armor`) 100.0))
  (set `self.Health` (`KismetMathLibrary.FClamp` (- (`self.Health`) _returnvalue) 0.0 100.0))
  (message `/Game/Blueprints/UI/UI_Interface.SetHealthBarPercent` (`WidgetComponent.GetUserWidgetObject` (`self.HealthBar_3D_WG`)) (/ (`self.Health`) 100.0))
  (`/Engine/EditorBlueprintResources/ActorMacros.Switch Has Authority`
    (:`Authority`
      (`self.DisplayDamageServer` _returnvalue))))

(event `OnLandedServer`
  ;[1 0 0] Damage
  ;;[1 1 1] On Landed
  (`self.OnLandedMulticast`))

(event `Armor > 0 Damage Client`
  (params (ArmorDamage :type "Float (double-precision)"))
  ;[1 0 0] Damage
  ;;[1 1 1] Health Damage
  (`self.Armor > 0 Damage Multicast` ArmorDamage))

(event `OnDamagePitchAudio`
  (params (Damage :type "Float (double-precision)"))
  ;[1 0 0] Damage
  (bind _returnvalue (`GameplayStatics.SpawnSoundAtLocation` "/Game/AUDIO/SFX_Damage/hit_fx_1_Cue.hit_fx_1_Cue" (`self.K2_GetActorLocation`) (struct) 1.0 1.0 0.0 null null))
  (`/Engine/EditorBlueprintResources/StandardMacros.IsValid` _returnvalue
    (:`Is Valid`
      (`AudioComponent.SetPitchMultiplier` _returnvalue (`KismetMathLibrary.MapRangeClamped` Damage 0.0 100.0 1.0 0.5)))))

(event `self.ReceiveRadialDamage`
  (params (DamageReceived :type "Float (single-precision)") (DamageType :type "DamageType Object Reference") (Origin :type "Vector Structure") (HitInfo :type "HitResult Structure (by ref)") (InstigatedBy :type "Controller Object Reference") (DamageCauser :type "Actor Object Reference"))
  ;[1 0 0] Damage
)

(fn `DisplayDamage`
  (params (Dmg :type "Float (double-precision)") (`Radial Hit Info` :type "HitResult Structure"))
  (bind (_x _y) (`KismetMathLibrary.BreakVector2D` (0.0 0.0)))
  (bind _returnvalue (`|CreateWidget` "/Game/Blueprints/UI/UI_DamageIndicator.UI_DamageIndicator_C"))
  (bind _asui_damage_indicator (cast `/Game/Blueprints/UI/UI_DamageIndicator` _returnvalue))
  (set `/Game/Blueprints/UI/UI_DamageIndicator.Damage_Integer` (`KismetMathLibrary.FTrunc` Dmg) _asui_damage_indicator)
  (if (== (`.HitBoneName` (`GameplayStatics.BreakHitResult` `Radial Hit Info`)) "head")
    (bind _damagetext (`/Game/Blueprints/UI/UI_DamageIndicator.DamageText` _asui_damage_indicator))
    (`TextBlock.SetFont` _damagetext (`/Game/Blueprints/UI/UI_DamageIndicator.CriticalDamageFontInfo` _asui_damage_indicator))
    (`TextBlock.SetColorAndOpacity` _damagetext (`/Game/Blueprints/UI/UI_DamageIndicator.CriticalDamageColor` _asui_damage_indicator))
    (else
      (`TextBlock.SetFont` _damagetext (`/Game/Blueprints/UI/UI_DamageIndicator.FontInfo` _asui_damage_indicator))
      (`TextBlock.SetColorAndOpacity` _damagetext (`/Game/Blueprints/UI/UI_DamageIndicator.DamageColor` _asui_damage_indicator))))
  (`UserWidget.AddToViewport` _returnvalue 0)
  (`Widget.SetRenderTranslation` _damagetext (- (`WidgetLayoutLibrary.ProjectWorldLocationToWidgetPosition` (`GameplayStatics.GetPlayerController` 0) (`SceneComponent.K2_GetComponentLocation` (`self.HealthBar_ROOT`))) (`KismetMathLibrary.MakeVector2D` (+ _x (`KismetMathLibrary.RandomFloatInRange` -50.0 50.0)) (+ _y (`KismetMathLibrary.RandomFloatInRange` -20.0 50.0))))))

(fn `GetPatrolPointsHolder`
  (returns (ReturnValue :type "/Game/Blueprints/CHARACTERS/NoobotAI/Blueprints/PatrolPointsHolderActor Object Reference"))
  (return (`self.PatrolPointsHolder`)))

(fn `GetShooterLocation`
  (returns (ReturnValue :type "Vector Structure"))
  (return (`SceneComponent.K2_GetComponentLocation` (`self.WeaponMuzzle`))))

(fn `OnRep_IsDead?`
  (if (`self.IsDead?`)
    (`/Engine/EditorBlueprintResources/StandardMacros.DoOnce` false :!label _label
      (:`Completed`
        (`self.IsDeadMulticast`)
        (`self.IsDeadServer`)))
    (else
      (goto _label :!via `Reset`))))

(fn `PortalRotationTracking`
  (bind _returnvalue (`self.K2_GetActorRotation`))
  (bind _returnvalue_2 (`self.GetController`))
  (bind _easemethod (`self.EaseMethod`))
  (bind _easerotation (`self.EaseRotation`))
  (bind _returnvalue_3 (`Controller.GetControlRotation` _returnvalue_2))
  (`|ExecutionSequence`
    (:`then_0`
      (`/Engine/EditorBlueprintResources/StandardMacros.IsValid` _returnvalue_2
        (:`Is Valid`
          (`Controller.SetControlRotation` _returnvalue_2 (`|EaseFunction` _easemethod _easerotation _returnvalue_3 (`KismetMathLibrary.MakeRotator` 0.0 (.pitch _returnvalue_3) (.yaw _returnvalue_3)))))))
    (:`then_1`
      (`self.K2_SetActorRotation` (`|EaseFunction` _easemethod _easerotation _returnvalue (`KismetMathLibrary.MakeRotator` 0.0 0.0 (.yaw _returnvalue)))))))

(fn `UpdateWalkSpeed`
  (params (Index :type "/Game/Blueprints/CHARACTERS/NoobotAI/Blueprints/Enums/StateEnum Enum" :default "NewEnumerator0"))
  (set `CharacterMovementComponent.MaxWalkSpeed` (select `/Game/Blueprints/CHARACTERS/NoobotAI/Blueprints/Enums/StateEnum` Index :`NewEnumerator0` (`self.PatrolSpeed`) :`NewEnumerator1` (`self.SearchSpeed`) :`NewEnumerator2` (`self.ChaseSpeed`)) (`self.CharacterMovement`))
  (return))

(fn `UserConstructionScript`)