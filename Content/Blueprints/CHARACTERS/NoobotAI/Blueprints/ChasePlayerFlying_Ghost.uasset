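; Behavior tree task that flies an EP2_GhostFlying pawn toward a point at an Elevation offset above the first player character.
; On each execution it picks a random speed and, unless the ghost is already within tolerance of that point, sets the CharacterMovement velocity straight at it.
; It steers by direct velocity rather than pathfinding and finishes successfully at once, so pursuit relies on repeated execution.
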(event `self.ReceiveExecuteAI`
  (params (OwnerController :type "AIController Object Reference") (ControlledPawn :type "Pawn Object Reference"))
  (set `self.Speed` (`KismetMathLibrary.RandomFloatInRange` 2000.0 2250.0))
  (bind _output_get (set `self.ControlledPawn` ControlledPawn))
  (bind _asep2_ghost_flying (cast `/Game/MISSIONS/EP2/Characters/EP2_GhostFlying` _output_get))
  (set `self.NewVar_1` (`Character.CharacterMovement` _asep2_ghost_flying))
  (if (not (== (`Actor.K2_GetActorLocation` (`self.ControlledPawn`)) (+ (`Actor.K2_GetActorLocation` (`GameplayStatics.GetPlayerCharacter` 0)) (`KismetMathLibrary.MakeVector` 0.0 0.0 (`self.Elevation`))) :`ErrorTolerance` 350.0))
    (set `MovementComponent.Velocity` (* (`KismetMathLibrary.GetDirectionUnitVector` (`Actor.K2_GetActorLocation` (`self.ControlledPawn`)) (+ (`Actor.K2_GetActorLocation` (`GameplayStatics.GetPlayerCharacter` 0)) (`KismetMathLibrary.MakeVector` 0.0 0.0 (`self.Elevation`)))) (`self.Speed`)) (`self.NewVar_1`)))
  (`self.FinishExecute` true))