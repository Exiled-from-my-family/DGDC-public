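; Actor that holds a list of patrol points, presumably for NoobotAI characters.
; On BeginPlay it converts each point in PatrolPoints from local to world space using the actor's transform, overwriting the array in place.
; Its construction script either saves the current location or, when LockRootLocation is set, snaps the actor back to that saved location to pin it in place.
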(event `self.ReceiveBeginPlay`
  ;[0.025 0.4029 1] Event Begin Play (Initialization)
  ;;[0 0 0] Transforming patrol locations from local space to world space
  (for (_array_element _array_index) (`self.Patrol Points`)
    (`KismetArrayLibrary.Array_Set` (`self.Patrol Points`) _array_index (`KismetMathLibrary.TransformLocation` (`self.GetTransform`) _array_element))))

(fn `UserConstructionScript`
  (`|ExecutionSequence`
    (:`then_0`
      (if (`self.Lock Root Location ?`)
        (`self.K2_SetActorLocation` (`self.Locked Location`))
        (else
          (set `self.Locked Location` (`self.K2_GetActorLocation`)))))))