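; Nailgun projectile for the NoobotAI character that explodes on its first hit and ignores collision with its instigator.
; At spawn it traces forward past tagged characters and projectiles, disabling physics simulation on its collision unless a PortalBP lies ahead.
; On hit it fires a radial impulse, applies splash damage doubled for head-bone hits, plays explosion effects, leaves a decal on non-projectile targets, then destroys itself.
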(event `self.ReceiveBeginPlay`
  (bind _collisioncomponent (`self.CollisionComponent`))
  (bind _returnvalue (`SceneComponent.K2_GetComponentLocation` _collisioncomponent))
  (bind _outactors (`GameplayStatics.GetAllActorsWithTag` "Character"))
  (bind _outactors_2 (`GameplayStatics.GetAllActorsWithTag` "Projectile"))
  (`KismetArrayLibrary.Array_Append` _outactors_2 _outactors)
  (bind _outhit (`KismetSystemLibrary.LineTraceSingle` _returnvalue (+ _returnvalue (* (`KismetMathLibrary.GetForwardVector` (`SceneComponent.K2_GetComponentRotation` _collisioncomponent)) 100000.0)) "TraceTypeQuery1" false _outactors_2))
  (if (not (`.bSuccess` (cast `/Game/kosm_fps_assets/Misc/Portal/PortalBP` (`.HitActor` (`GameplayStatics.BreakHitResult` _outhit)) :!pure true)))
    (`PrimitiveComponent.SetSimulatePhysics` (`self.CollisionComponent`) false)))

(event `self.ReceiveHit`
  (params (MyComp :type "PrimitiveComponent Object Reference") (Other :type "Actor Object Reference") (OtherComp :type "PrimitiveComponent Object Reference") (bSelfMoved :type Boolean) (HitLocation :type "Vector Structure") (HitNormal :type "Vector Structure") (NormalImpulse :type "Vector Structure") (Hit :type "HitResult Structure (by ref)"))
  (bind (_bblockinghit _binitialoverlap _time _distance _location _impactpoint _normal _impactnormal _physmat _hitactor _hitcomponent _hitbonename) (`GameplayStatics.BreakHitResult` Hit))
  ;[0.3687 0.5739 1] Begin Hit Event - Impulse and Splash Damage
  (`/Engine/EditorBlueprintResources/StandardMacros.DoOnce` false
    (:`Completed`
      (`RadialForceComponent.FireImpulse` (`self.RadialForce`))
      (if (== _hitbonename "head")
        (`GameplayStatics.ApplyRadialDamage` :`BaseDamage` 32.0 :`Origin` HitLocation :`DamageRadius` 140.0 :`DamageCauser` null :`InstigatedByController` (`self.GetInstigatorController`))
        (else
          (`GameplayStatics.ApplyRadialDamage` :`BaseDamage` 16.0 :`Origin` HitLocation :`DamageRadius` 140.0 :`DamageCauser` null :`InstigatedByController` (`self.GetInstigatorController`))))
      (`GameplayStatics.SpawnEmitterAtLocation` "/Game/kosm_fps_assets/Misc/Particles/P_Explosion.P_Explosion" (`self.K2_GetActorLocation`) (struct) (0.5 0.5 0.5))
      (`GameplayStatics.PlaySoundAtLocation` "/Game/AUDIO/SFX_Weapons/Weap_GrenadeLauncher/SC_Explosion.SC_Explosion" (`SceneComponent.K2_GetComponentLocation` (`self.RadialForce`)) (struct) 0.75 1.0 0.0 null null null)
      (if (not (`self.ActorHasTag` _hitactor "Projectile"))
        (bind _returnvalue (`GameplayStatics.SpawnDecalAttached` "/Game/kosm_fps_assets/Misc/Materials/BulletHole001.BulletHole001" (7.0 7.0 7.0) OtherComp "None" (`KismetMathLibrary.InverseTransformLocation` (`SceneComponent.K2_GetComponentToWorld` OtherComp) HitLocation) (`KismetMathLibrary.Conv_VectorToRotator` _normal) "SnapToTargetIncludingScale" 30.0))
        (`DecalComponent.SetFadeScreenSize` _returnvalue 0.001))
      (`self.K2_DestroyActor`))))

(fn `IgnoreActorWhenMoving`
  (`PrimitiveComponent.IgnoreActorWhenMoving` (`self.CollisionComponent`) (`self.GetInstigator`) true))

(fn `UserConstructionScript`
  (`self.IgnoreActorWhenMoving`))