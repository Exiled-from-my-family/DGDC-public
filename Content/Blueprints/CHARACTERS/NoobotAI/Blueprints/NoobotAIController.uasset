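; AI controller for the Noobot that starts its behavior tree on possess and seeds the blackboard with nailgun selection and patrol route.
; Perception tracks the two fpsMovementCharacter types: sight sets the enemy key, clearing it after a timeout or on death.
; Hearing stores a suspect location only while no enemy is set.
; A helper supplies patrol locations, falling back to the pawn's position, though its index-advance math is unwired.
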(event `self.ReceivePossess`
  (params (PossessedPawn :type "Pawn Object Reference"))
  ;[1 0.8031 0.3206] On Begin Play
  (bind _blackboardcomponent (`self.UseBlackboard` "/Game/Blueprints/CHARACTERS/NoobotAI/Blueprints/NoobotBlackboard.NoobotBlackboard"))
  (`BlackboardComponent.SetValueAsBool` _blackboardcomponent (`self.NailgunSelectedKeyName`) true) ; SEP 14 2020 NAILGUN SELECTED BY DEFAULT
  (`self.RunBehaviorTree` "/Game/Blueprints/CHARACTERS/NoobotAI/Blueprints/NoobotBT.NoobotBT")
  (bind _returnvalue (message `/Game/Blueprints/CHARACTERS/NoobotAI/Blueprints/AI_Interface.GetPatrolPointsHolder` (`self.K2_GetPawn`)))
  (`self.Update Patrol Points Actor Key` _returnvalue))

(event `Clear Target Enemy`
  ;[1 0.3358 0.2207] On Perception Updated
  (`self.Update Sight Keys` null)
  (message `/Game/Blueprints/CHARACTERS/NoobotAI/Blueprints/AI_Interface.UpdateState` (`self.K2_GetPawn`)))

(event `self.AIPerception.OnTargetPerceptionUpdated`
  (params (Actor :type "Actor Object Reference") (Stimulus :type "AIStimulus Structure"))
  (bind ((`StimulusLocation` _stimuluslocation) (`bSuccessfullySensed` _bsuccessfullysensed)) (break `AIStimulus` (`self.CurrentAIStimulus_Ref`)))
  ;[1 0.3358 0.2207] On Perception Updated
  (if (or (`.bSuccess` (cast `/Game/Blueprints/CHARACTERS/fpsMovementCharacter_light_1_vq3` Actor :!pure true)) (`.bSuccess` (cast `/Game/Blueprints/CHARACTERS/fpsMovementCharacter_light_2_cpma` Actor :!pure true)))
    (bind _output_get (set `self.SensedEnemy_Ref` Actor))
    (bind _return_value (message `/Game/Blueprints/CHARACTERS/Character_Interface.IsAlive` _output_get))
    (if _return_value
      (bind _info (`AIPerceptionComponent.GetActorsPerception` (`self.AIPerception`) (`self.SensedEnemy_Ref`)))
      (for (_array_element _array_index) (`.LastSensedStimuli` (break `ActorPerceptionBlueprintInfo` _info))
        (set `self.CurrentAIStimulus_Ref` _array_element)
        (switch `/Game/Blueprints/CHARACTERS/NoobotAI/Blueprints/SensesEnum` (cast `/Game/Blueprints/CHARACTERS/NoobotAI/Blueprints/SensesEnum` (`KismetMathLibrary.Conv_IntToByte` _array_index))
          (:`NewEnumerator0`
            (if (`.bSuccessfullySensed` (break `AIStimulus` (`self.CurrentAIStimulus_Ref`)))
              (`KismetSystemLibrary.K2_ClearAndInvalidateTimerHandle` (`self.LooseSightTimerHandle`))
              (`self.Update Sight Keys` (`self.SensedEnemy_Ref`))
              (`self.Update Hearing Keys` false)
              (message `/Game/Blueprints/CHARACTERS/NoobotAI/Blueprints/AI_Interface.UpdateState` (`self.K2_GetPawn`))
              (else
                (bind _returnvalue (`KismetSystemLibrary.K2_SetTimerDelegate` (delegate `Clear Target Enemy`) (`self.Sight Loss Timeout`)))
                (set `self.LooseSightTimerHandle` _returnvalue))))
          (:`NewEnumerator1`
            (`/Engine/EditorBlueprintResources/StandardMacros.IsValid` (`self.GetEnemyKeyAsObject`)
              (:`Is Not Valid`
                (if _bsuccessfullysensed
                  (`self.Update Hearing Keys` true _stimuluslocation)
                  (message `/Game/Blueprints/CHARACTERS/NoobotAI/Blueprints/AI_Interface.UpdateState` (`self.K2_GetPawn`))))))))
      (else
        (`/Engine/EditorBlueprintResources/StandardMacros.IsValid` (`self.GetEnemyKeyAsObject`)
          (:`Is Valid`
            (`self.Update Sight Keys` null)
            (`self.Update Hearing Keys` false)
            (message `/Game/Blueprints/CHARACTERS/NoobotAI/Blueprints/AI_Interface.UpdateState` (`self.K2_GetPawn`))))))))

(fn `Get Next Patrol Point`
  (returns (`Return Value` :type "Vector Structure"))
  (locals (PatrolPoints_Local :type "Array of Vector Structure") (NextPatrolPoint_Local :type "Vector Structure"))
  (bind (_returnvalue _isvalid) (`self.GetPatrolPointsHolder`)) ; Getting Patrol Points \nHolder From Blackboard
  (if _isvalid
    (bind _output_get (set `local.PatrolPoints_Local` (`/Game/Blueprints/CHARACTERS/NoobotAI/Blueprints/PatrolPointsHolderActor.Patrol Points` _returnvalue)))
    (if (> (`KismetArrayLibrary.Array_Length` _output_get) 0)
      (set `self.CurrentPatrolPointIndex` (mod (+ (`self.CurrentPatrolPointIndex`) 1) (`KismetArrayLibrary.Array_Length` (`local.PatrolPoints_Local`))))
      (set `local.NextPatrolPoint_Local` (`|GetArrayItem` (`local.PatrolPoints_Local`) (`self.CurrentPatrolPointIndex`)))
      (else
        (set `local.NextPatrolPoint_Local` (`self.K2_GetActorLocation` (`self.K2_GetPawn`)) :!label _label)))
    (else
      (goto _label)))
  (return (`local.NextPatrolPoint_Local`)) ; Returning Next Patrol Point Location
)

(fn `GetEnemyKeyAsObject`
  (returns (ReturnValue :type "Object Object Reference"))
  (return (`BlackboardComponent.GetValueAsObject` (`AIBlueprintHelperLibrary.GetBlackboard` null) (`self.EnemyKeyName`))))

(fn `GetPatrolPointsHolder`
  (returns (ReturnValue :type "/Game/Blueprints/CHARACTERS/NoobotAI/Blueprints/PatrolPointsHolderActor Object Reference") (IsValid :type Boolean))
  (locals (`IsValid?` :type Boolean))
  (bind (_aspatrol_points_holder_actor _bsuccess) (cast `/Game/Blueprints/CHARACTERS/NoobotAI/Blueprints/PatrolPointsHolderActor` (`BlackboardComponent.GetValueAsObject` (`AIBlueprintHelperLibrary.GetBlackboard` null) (`self.PatrolPointsHolderKeyName`)) :!pure true))
  (return _aspatrol_points_holder_actor _bsuccess))

(fn `Update Hearing Keys`
  (params (`NoiseHeard?` :type Boolean) (`Noise Location` :type "Vector Structure"))
  (`BlackboardComponent.SetValueAsBool` (`AIBlueprintHelperLibrary.GetBlackboard` null) (`self.NoiseHeardKeyName`) `NoiseHeard?`)
  (if `NoiseHeard?`
    (`BlackboardComponent.SetValueAsVector` (`AIBlueprintHelperLibrary.GetBlackboard` null) (`self.SuspectLocationKeyName`) `Noise Location`)))

(fn `Update Patrol Points Actor Key`
  (params (NewPatrolPointsHolder :type "Object Object Reference"))
  (`BlackboardComponent.SetValueAsObject` (`AIBlueprintHelperLibrary.GetBlackboard` null) (`self.PatrolPointsHolderKeyName`) NewPatrolPointsHolder))

(fn `Update Sight Keys`
  (params (ObjectValue :type "Object Object Reference"))
  (`BlackboardComponent.SetValueAsObject` (`AIBlueprintHelperLibrary.GetBlackboard` null) (`self.EnemyKeyName`) ObjectValue))

(fn `UserConstructionScript`)