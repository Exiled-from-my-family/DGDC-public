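; DebugSphere is a Noobot AI debug node that visualizes a Blackboard location in the world.
; When debugging is enabled, each tick reads the vector under LocationKey and draws a vertical debug cylinder centered on it, despite the sphere name.
; Radius, height, segments and color come from variables, and each shape lasts slightly longer than the tick interval so the display stays continuous.
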(event `self.ReceiveTick`
  (params (OwnerActor :type "Actor Object Reference") (DeltaSeconds :type "Float (single-precision)"))
  (bind _returnvalue (`BTFunctionLibrary.GetBlackboardValueAsVector` (`self.LocationKey`)))
  (bind _returnvalue_2 (`KismetMathLibrary.MakeVector` 0.0 0.0 (`self.Height`)))
  (if (`self.DebugEnabled`)
    (`KismetSystemLibrary.DrawDebugCylinder` (- _returnvalue _returnvalue_2) (+ _returnvalue _returnvalue_2) (`self.Radius`) (`self.Segments`) (`self.Color`) (+ DeltaSeconds 0.2))))