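; Game state that tracks time spent on the game instance, refreshes the scoreboard and announces the player's killstreaks.
; Each score update matching the player's name increments a chain that a retriggerable delay resets after a few seconds without kills, while negative scores decrement it to prevent friendly-fire streaks.
; The chain count selects the killstreak message, shown after clearing older killstreak widgets, and a slightly delayed announcer sound.
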(event `self.ReceiveBeginPlay`
  (set `self.instance` (`/Game/Blueprints/NewFunctionLibrary.dead game instance PURE`)))

(event `self.ReceiveTick`
  (params (DeltaSeconds :type "Float (single-precision)"))
  (bind _instance (`self.instance`))
  (set `/Game/Blueprints/DeadGaemInstance.Time spent` (+ (`/Game/Blueprints/DeadGaemInstance.Time spent` _instance) DeltaSeconds) _instance))

(event `update`
  (params (name :type String) (score :type Integer))
  (bind _player_chain (`self.player chain`))
  (`self.send` (`self.Score Board`))
  (bind _player (`/Game/Blueprints/NewFunctionLibrary.get player`))
  (if (< score 0)
    (`/Engine/EditorBlueprintResources/StandardMacros.DecrementInt` _player_chain :!pinned true) ; to prevent friendly killstreaks
    (elif (and (`KismetStringLibrary.EqualEqual_StrStr` name (`/Game/Blueprints/CHARACTERS/fpsMovementCharacter_light_1_vq3.player's name` _player)) (> score 0))
      (bind _result (`/Engine/EditorBlueprintResources/StandardMacros.IncrementInt` _player_chain)
        (:`  `
          (`|ExecutionSequence`
            (:`then_0`
              (if (> _player_chain 1)
                (bind _foundwidgets (`WidgetBlueprintLibrary.GetAllWidgetsOfClass` "/Game/Blueprints/UI/UI_Gameplay/UI_Killstreak_message.UI_Killstreak_message_C"))
                (`Widget.RemoveFromParent` _foundwidgets)
                (`KismetSystemLibrary.Delay` 0.01)
                (`/Game/Blueprints/NewFunctionLibrary.killstreak` (select `int` _result :`0` "" :`1` "" :`2` "DOUBLE KILL!" :`3` "TRIPLE KILL!" :`4` "QUAD KILL!" :`5` "SERIAL KILLER!" :`6` "GENOCIDAL" :!type "Text")))
              (`KismetSystemLibrary.RetriggerableDelay` 4.0)
              (set `self.player chain` 0))
            (:`then_1`
              (`KismetSystemLibrary.Delay` 0.2)
              (`GameplayStatics.PlaySound2D` (select `int` _result :`0` null :`1` null :`2` "/Game/AUDIO/SFX_Announcer/SW_An_Killstreak_1.SW_An_Killstreak_1" :`3` "/Game/AUDIO/SFX_Announcer/SW_An_Killstreak_2.SW_An_Killstreak_2" :`4` "/Game/AUDIO/SFX_Announcer/SW_An_Killstreak_3.SW_An_Killstreak_3" :`5` "/Game/AUDIO/SFX_Announcer/SW_An_Killstreak_4.SW_An_Killstreak_4" :`6` "/Game/AUDIO/SFX_Announcer/SW_An_Killstreak_5.SW_An_Killstreak_5" :!type "SoundBase Object Reference") 1.0 1.0 0.0 null null))))))))

(fn `UserConstructionScript`)