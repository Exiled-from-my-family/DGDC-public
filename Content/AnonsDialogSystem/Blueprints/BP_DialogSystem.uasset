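; Dialog component for an NPC owner that runs branching conversations from DataTable rows in a W_DialogBox widget.
; Talk opens the UI, locks player input and loads the current row, showing text, voice, optional camera blend and up to four W_DialogEntry responses.
; Dialog broadcasts event IDs and loads the matching row, with SwitchID selecting alternate answers.
; The "quit" ID closes the UI, restores input and player visuals, and stops NPC montages.
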(event `Talk`
  (`self.CreateDialogUI` null (1000.0 400.0) (0.0 0.0) (struct) (struct :`A` 0.5))
  (`self.AddDataTable` "/Game/AnonsDialogSystem/Data/DT_Dialog.DT_Dialog" (`self.DataTableRowID`)))

(event `/Game/AnonsDialogSystem/Blueprints/BPI_DialogInterface.Dialog`
  (params (EventID :type Name) (SwitchID :type Integer) (DialogText :type Text))
  (`self.event id dispatch` EventID)
  (bind _success (`self.GlobalDialogEvent` EventID))
  (if (not _success)
    (`self.AddDataTable` (`self.DataTable`) EventID SwitchID)))

(event `StopAnim`
  (params (Mesh :type "SkeletalMeshComponent Object Reference") (Target :type "AnimInstance Object Reference") (Montage :type "AnimMontage Object Reference"))
  ;[0 0 0] Ends dialog anim
  (`AnimInstance.Montage_Stop` Target 0.25 Montage)
  (`KismetSystemLibrary.Delay` 0.25)
  (`SkeletalMeshComponent.SetAnimationMode` Mesh "AnimationBlueprint"))

(fn `AddCameraAngle`
  (params (CameraActorTarget :type "Actor Object Reference") (CameraBlendTime :type "Float (double-precision)" :default 1.0) (CameraDistence :type "Float (double-precision)" :default 300.0) (CameraHight :type "Float (double-precision)" :default 70.0) (CameraAngle :type "Float (double-precision)") (`CameraAttach?` :type Boolean))
  (returns (DialogSystem :type "/Game/AnonsDialogSystem/Blueprints/BP_DialogSystem Object Reference"))
  (locals (CameraTarget :type "Actor Object Reference"))
  (bind _returnvalue (`self.GetOwner`))
  (bind _oldscenecamera (`self.OldSceneCamera`))
  (bind _cameratarget (`local.CameraTarget`))
  (bind _scenecamera (`self.SceneCamera`))
  (bind _dialogbox (`self.DialogBox`))
  (bind _returnvalue_2 (+ (`Actor.K2_GetActorLocation` _cameratarget) (`KismetMathLibrary.MakeVector` 0.0 0.0 CameraHight)))
  (bind _returnvalue_3 (+ _returnvalue_2 (`KismetMathLibrary.RotateAngleAxis` (* (`Actor.GetActorForwardVector` _cameratarget) CameraDistence) CameraAngle (0.0 0.0 1.0))))
  ;[0 0 0] Creates camera actor
  (if (not (and (== CameraActorTarget (`self.Target`)) (== (`KismetMathLibrary.MakeVector` CameraDistence CameraHight CameraAngle) (`self.CameraSetting`))))
    (set `self.CameraSetting` (`KismetMathLibrary.MakeVector` CameraDistence CameraHight CameraAngle))
    (`/Engine/EditorBlueprintResources/StandardMacros.IsValid` CameraActorTarget
      (:`Is Valid`
        (set `local.CameraTarget` CameraActorTarget)
        (set `self.Target` CameraActorTarget))
      (:`Is Not Valid`
        (set `local.CameraTarget` _returnvalue)
        (set `self.Target` _returnvalue)))
    (`/Engine/EditorBlueprintResources/StandardMacros.IsValid` _oldscenecamera
      (:`Is Valid`
        (`Actor.K2_DestroyActor` _oldscenecamera))
      (:`Is Not Valid`
        _))
    (`/Engine/EditorBlueprintResources/StandardMacros.IsValid` _scenecamera
      (:`Is Valid`
        (set `self.OldSceneCamera` _scenecamera))
      (:`Is Not Valid`
        _))
    (bind _output_get (set `/Game/AnonsDialogSystem/UI/W_DialogBox.CameraBlendTime` CameraBlendTime (`self.DialogBox`)))
    (bind _returnvalue_4 (`|SpawnActorFromClass` "/Script/Engine.CameraActor" (`KismetMathLibrary.MakeTransform` _returnvalue_3 (`KismetMathLibrary.FindLookAtRotation` _returnvalue_3 _returnvalue_2)) "AlwaysSpawn" "OverrideRootScale" null null))
    (`CameraComponent.SetConstraintAspectRatio` (`CameraActor.CameraComponent` _returnvalue_4) false)
    (`PlayerController.SetViewTargetWithBlend` (`GameplayStatics.GetPlayerController` 0) _returnvalue_4 _output_get "VTBlend_Linear" 0.0 false)
    (bind _output_get_2 (set `self.SceneCamera` _returnvalue_4))
    (set `/Game/AnonsDialogSystem/UI/W_DialogBox.SceneCamera` _output_get_2 _dialogbox)
    (set `/Game/AnonsDialogSystem/UI/W_DialogBox.OldSceneCamera` (`self.OldSceneCamera`) _dialogbox)
    ;[0 0 0] Attaches camera to target
    (if `CameraAttach?`
      (`/Engine/EditorBlueprintResources/StandardMacros.IsValid` (`local.CameraTarget`)
        (:`Is Valid`
          (`Actor.K2_AttachToActor` _returnvalue_4 (`local.CameraTarget`) "None" "KeepWorld" "KeepWorld" "KeepWorld" true))
        (:`Is Not Valid`
          _)))
    (return self)))

(fn `AddDataTable`
  (params (DataTable :type "DataTable Object Reference") (RowName :type Name) (SwitchID :type Integer))
  (bind _returnvalue (== SwitchID 4444))
  (bind _returnvalue_2 (== SwitchID 1111))
  (bind _returnvalue_3 (== SwitchID 2222))
  (bind _returnvalue_4 (== SwitchID 3333))
  (bind _showdebug_ (`self.ShowDebug?`))
  ;[0 0 0] Reads DataTable
  (bind _outrownames (`DataTableFunctionLibrary.GetDataTableRowNames` DataTable))
  (bind _returnvalue_5 (!= (`KismetArrayLibrary.Array_Find` _outrownames RowName) -1))
  (if _returnvalue_5
    (set `self.DataTableRowID` RowName)
    (bind _returnvalue_6 (`|GetDataTableRow` DataTable (select `bool` _returnvalue_5 :`false` (`self.DataTableRowID`) :`true` RowName) :!label _label)
      (:`then`
        _)
      (:`RowNotFound`
        (`KismetSystemLibrary.PrintString` "Error: invalid table name" _showdebug_ _showdebug_ (struct :`R` 1.0 :`A` 1.0))
        (return)))
    (elif (== RowName "quit")
      (return)
      (else
        (goto _label))))
  (bind (_dialogimage _dialogname _dialogtext _dialogaudio _dialogeventid _dialogeventdelay _typingdelay _response1 _response2 _response3 _response4 _responseevent1 _responseevent2 _responseevent3 _responseevent4 _responseaudio1 _responseaudio2 _responseaudio3 _responseaudio4 _answer1 _answer2 _answer3 _answer4 _answerevent1 _answerevent2 _answerevent3 _answerevent4 _answeraudio1 _answeraudio2 _answeraudio3 _answeraudio4 _isnpcdialogclickable_ _cleardialogresponses_ _cameraangle) (break `/Game/AnonsDialogSystem/Data/Dialog_Struct` _returnvalue_6))
  (if (not (== _cameraangle 0.0))
    (`self.AddCameraAngle` null 1.0 300.0 70.0 _cameraangle))
  (`self.AddDialog` _dialogimage _dialogname (select `bool` _returnvalue_2 :`false` (select `bool` _returnvalue_3 :`false` (select `bool` _returnvalue_4 :`false` (select `bool` _returnvalue :`false` _dialogtext :`true` _answer4) :`true` _answer3) :`true` _answer2) :`true` _answer1) (select `bool` _returnvalue_2 :`false` (select `bool` _returnvalue_3 :`false` (select `bool` _returnvalue_4 :`false` (select `bool` _returnvalue :`false` _dialogeventid :`true` _answerevent4) :`true` _answerevent3) :`true` _answerevent2) :`true` _answerevent1) (struct :`A` 1.0) (struct :`R` 0.498039 :`G` 0.498039 :`B` 0.498039 :`A` 1.0) (struct :`R` 1.0 :`G` 1.0 :`B` 1.0 :`A` 1.0) null null (select `bool` _returnvalue_2 :`false` (select `bool` _returnvalue_3 :`false` (select `bool` _returnvalue_4 :`false` (select `bool` _returnvalue :`false` _dialogaudio :`true` _answeraudio4) :`true` _answeraudio3) :`true` _answeraudio2) :`true` _answeraudio1) _dialogeventdelay _typingdelay (select `bool` (> _typingdelay 0.0) :`true` "/Game/AnonsDialogSystem/Demo/Sound/Cue/S_Keyboard_typing_Cue.S_Keyboard_typing_Cue" :!type "SoundBase Object Reference") _isnpcdialogclickable_ _cleardialogresponses_)
  (for (_array_element _array_index) (`|MakeArray` (`KismetTextLibrary.NotEqual_TextText` _response1 "") (`KismetTextLibrary.NotEqual_TextText` _response2 "") (`KismetTextLibrary.NotEqual_TextText` _response3 "") (`KismetTextLibrary.NotEqual_TextText` _response4 ""))
    (if (== _array_element true)
      (`self.AddResponse` "" (select `int` _array_index :`0` _response1 :`1` _response2 :`2` _response3 :`3` _response4) (select `int` _array_index :`0` _responseevent1 :`1` _responseevent2 :`2` _responseevent3 :`3` _responseevent4) (select `int` _array_index :`0` (select `bool` (`KismetTextLibrary.NotEqual_TextText` _answer1 "") :`true` 1111) :`1` (select `bool` (`KismetTextLibrary.NotEqual_TextText` _answer2 "") :`true` 2222) :`2` (select `bool` (`KismetTextLibrary.NotEqual_TextText` _answer3 "") :`true` 3333) :`3` (select `bool` (`KismetTextLibrary.NotEqual_TextText` _answer4 "") :`true` 4444)) (struct) null (select `int` _array_index :`0` _responseaudio1 :`1` _responseaudio3 :`2` _responseaudio2 :`3` _responseaudio4) (struct :`R` 0.328125 :`A` 1.0))))
  (return))

(fn `AddDialog`
  (params (NPCImage :type "Texture2D Object Reference") (NPCName :type Text) (Dialog :type Text) (DialogID :type Name) (NameColor :type "LinearColor Structure") (DialogHoveredColor :type "LinearColor Structure") (DialogNormalColor :type "LinearColor Structure" :default (struct :`A` 1.0)) (DialogFont :type "Font Object Reference") (DialogAnim :type "AnimMontage Object Reference") (DialogSound :type "SoundBase Object Reference") (DialogEventDelay :type "Float (double-precision)") (DialogTypingDelay :type "Float (double-precision)" :default 0.02) (DialogTypingSound :type "SoundBase Object Reference") (`IsDialogClickable?` :type Boolean) (`ClearDialogResponses?` :type Boolean :default true))
  (returns (DialogSystem :type "/Game/AnonsDialogSystem/Blueprints/BP_DialogSystem Object Reference") (DelayValue :type "Float (double-precision)"))
  (bind (_r _g _b) (break `LinearColor` NameColor))
  (bind _showdebug_ (`self.ShowDebug?`))
  (bind _dialogbox (`self.DialogBox`))
  (bind _dialogbox_2 (`self.DialogBox`))
  (bind _dialogbox_3 (`self.DialogBox`))
  (bind _npcdialogtext (`/Game/AnonsDialogSystem/UI/W_DialogBox.NPCDialogText` _dialogbox_2))
  (bind _npcdialogoverlay (`/Game/AnonsDialogSystem/UI/W_DialogBox.NPCDialogOverlay` (`self.DialogBox`)))
  (bind _returnvalue (* (`KismetStringLibrary.Len` (`KismetTextLibrary.Conv_TextToString` Dialog)) DialogTypingDelay))
  (bind _returnvalue_2 (`Widget.IsVisible` _npcdialogoverlay))
  (bind (_fontobject _fontmaterial _outlinesettings _typefacefontname _size) (break `SlateFontInfo` (`TextBlock.Font` (`/Game/AnonsDialogSystem/UI/W_DialogBox.NPCDialogText` _dialogbox_2))))
  ;[0 0 0] Adds NPC dialog text to main dialog UI
  (if (> (`KismetStringLibrary.Len` (`KismetTextLibrary.Conv_TextToString` Dialog)) 0)
    (if (not _returnvalue_2)
      (`Widget.SetVisibility` _npcdialogoverlay "Visible"))
    (if (`KismetSystemLibrary.IsValid` DialogAnim) :!label _label
      (bind _ascharacter (cast `Character` (`self.NPCReference`))
        (:`then`
          (bind _mesh (`Character.Mesh` _ascharacter))
          (if (not (`AnimInstance.Montage_IsPlaying` (`SkeletalMeshComponent.GetAnimInstance` _mesh) DialogAnim))
            (`SkeletalMeshComponent.PlayAnimation` _mesh DialogAnim true)))
        (:`CastFailed`
          (return null 0.0))))
    (else
      (`/Engine/EditorBlueprintResources/StandardMacros.IsValid` DialogSound
        (:`Is Valid`
          (if _returnvalue_2
            (`Widget.SetVisibility` _npcdialogoverlay "Collapsed")
            (goto _label)
            (else
              (goto _label))))
        (:`Is Not Valid`
          (`Widget.RemoveFromParent` (`self.DialogBox`))
          (`WidgetBlueprintLibrary.SetInputMode_GameOnly` (`GameplayStatics.GetPlayerController` 0))
          (`KismetSystemLibrary.PrintString` "Error: no dialog or voice found" _showdebug_ _showdebug_)
          (return null 0.0)))))
  (if (not (not `ClearDialogResponses?`))
    (`PanelWidget.ClearChildren` (`/Game/AnonsDialogSystem/UI/W_DialogBox.DialogSBox` _dialogbox)))
  (set `/Game/AnonsDialogSystem/UI/W_DialogBox.TextColorHovered` DialogHoveredColor _dialogbox_2)
  (set `/Game/AnonsDialogSystem/UI/W_DialogBox.TextColorNormal` DialogNormalColor _dialogbox_2)
  (`TextBlock.SetColorAndOpacity` _npcdialogtext (make `SlateColor` DialogNormalColor))
  (`TextBlock.SetColorAndOpacity` (`/Game/AnonsDialogSystem/UI/W_DialogBox.NPCNameText` _dialogbox_2) (make `SlateColor` (`KismetMathLibrary.SelectColor` (struct :`A` 1.0) NameColor (and (== _r 0.0) (== _g 0.0) (== _b 0.0)))))
  (`TextBlock.SetFont` _npcdialogtext (make `SlateFontInfo` (`KismetMathLibrary.SelectObject` DialogFont _fontobject (`KismetSystemLibrary.IsValid` DialogFont)) _fontmaterial _outlinesettings _typefacefontname _size))
  (`/Engine/EditorBlueprintResources/StandardMacros.IsValid` NPCImage
    (:`Is Valid`
      (`Image.SetBrushFromTexture` (`/Game/AnonsDialogSystem/UI/W_DialogBox.NPCImage` _dialogbox_2) NPCImage false))
    (:`Is Not Valid`
      _))
  (set `/Game/AnonsDialogSystem/UI/W_DialogBox.DialogClickable?` `IsDialogClickable?` _dialogbox_3)
  (set `/Game/AnonsDialogSystem/UI/W_DialogBox.NPCDialog` Dialog _dialogbox_3)
  (set `/Game/AnonsDialogSystem/UI/W_DialogBox.DialogEventDelay` DialogEventDelay _dialogbox)
  (set `/Game/AnonsDialogSystem/UI/W_DialogBox.NPCDialogID` DialogID _dialogbox_3)
  (set `/Game/AnonsDialogSystem/UI/W_DialogBox.TypingSound` DialogTypingSound _dialogbox_3)
  (`Widget.SetVisibility` (`/Game/AnonsDialogSystem/UI/W_DialogBox.NPCDialogVBox` _dialogbox_3) "Visible")
  (`GameplayStatics.SpawnSoundAtLocation` DialogSound (`Actor.K2_GetActorLocation` (`self.GetOwner`)) (struct) 1.0 1.0 0.0 null null)
  (`TextBlock.SetText` (`/Game/AnonsDialogSystem/UI/W_DialogBox.NPCNameText` _dialogbox_3) NPCName) ; Sets NPC Name
  (`/Game/AnonsDialogSystem/UI/W_DialogBox.SetNPCDialog` _dialogbox_3 DialogTypingDelay)
  (return self (select `bool` (> DialogEventDelay 0.0) :`false` (select `bool` (!= _returnvalue 0.0) :`false` (select `bool` (`KismetSystemLibrary.IsValid` DialogSound) :`true` (`SoundBase.Duration` DialogSound)) :`true` _returnvalue) :`true` DialogEventDelay)))

(fn `AddResponse`
  (params (Name :type Text) (ResponseDialog :type Text) (EventID :type Name :default "None") (SwitchID :type Integer) (NameColor :type "LinearColor Structure") (ResponseFont :type "Font Object Reference") (ResponseVoice :type "SoundBase Object Reference") (TextColorHovered :type "LinearColor Structure" :default (struct :`A` 1.0)) (TextColorNormal :type "LinearColor Structure" :default (struct :`A` 1.0)) (BtnHoveredImage :type "Texture2D Object Reference") (BtnNormalImage :type "Texture2D Object Reference") (EnableEventDelay :type "Float (double-precision)"))
  (returns (DialogSystem :type "/Game/AnonsDialogSystem/Blueprints/BP_DialogSystem Object Reference"))
  (bind (_r _g _b) (break `LinearColor` NameColor))
  (bind _dialogbox (`self.DialogBox`))
  (bind _dialogsbox (`/Game/AnonsDialogSystem/UI/W_DialogBox.DialogSBox` (`self.DialogBox`)))
  ;[0 0 0] Adds a dialog button to the main dialog UI
  (`self.event id dispatch` EventID)
  (set `/Game/AnonsDialogSystem/UI/W_DialogBox.Name` Name (`self.DialogBox`))
  (bind _returnvalue (`|CreateWidget` "/Game/AnonsDialogSystem/UI/W_DialogEntry.W_DialogEntry_C" (`GameplayStatics.GetPlayerController` 0) EventID SwitchID ResponseDialog ResponseVoice (`self.NPCReference`) self EnableEventDelay TextColorHovered TextColorNormal BtnHoveredImage BtnNormalImage (`self.ShowDebug?`)))
  (`TextBlock.SetColorAndOpacity` (`/Game/AnonsDialogSystem/UI/W_DialogBox.DialogNameText` _dialogbox) (make `SlateColor` (`KismetMathLibrary.SelectColor` (struct :`A` 1.0) NameColor (and (== _r 0.0) (== _g 0.0) (== _b 0.0)))))
  (bind _text (`/Game/AnonsDialogSystem/UI/W_DialogEntry.Text` _returnvalue))
  (bind (_fontobject _fontmaterial _outlinesettings _typefacefontname _size) (break `SlateFontInfo` (`TextBlock.Font` _text)))
  (`TextBlock.SetFont` _text (make `SlateFontInfo` (`KismetMathLibrary.SelectObject` ResponseFont _fontobject (`KismetSystemLibrary.IsValid` ResponseFont)) _fontmaterial _outlinesettings _typefacefontname _size))
  (bind _button (`/Game/AnonsDialogSystem/UI/W_DialogEntry.Button` _returnvalue))
  (`PanelWidget.AddChild` _dialogsbox _button)
  (`/Game/AnonsDialogSystem/UI/W_DialogBox.MakeResponseBoxVisible` _dialogbox)
  (`/Game/AnonsDialogSystem/UI/W_DialogEntry.Highlight` _returnvalue)
  (if (== (`PanelWidget.GetChildIndex` _dialogsbox _button) 0)
    (`Widget.SetKeyboardFocus` _button)
    (`Widget.SetUserFocus` _button (`GameplayStatics.GetPlayerController` 0)))
  (return self))

(fn `CreateDialogUI`
  (params (GUITexture :type "Texture2D Object Reference") (MainSize :type "Vector2D Structure" :default (1000.0 400.0)) (MainTranslation :type "Vector2D Structure") (MainBorderColor :type "LinearColor Structure" :default (struct)) (NPCBorderColor :type "LinearColor Structure" :default (struct)) (bShowMouseCursor :type Boolean :default true) (`bShowDebug?` :type Boolean))
  (returns (DialogSystem :type "/Game/AnonsDialogSystem/Blueprints/BP_DialogSystem Object Reference"))
  (bind _returnvalue (`GameplayStatics.GetPlayerController` 0))
  (bind _returnvalue_2 (`self.GetOwner`))
  (bind (_x _y) (`KismetMathLibrary.BreakVector2D` MainSize))
  (bind _dialogbox (`self.DialogBox`))
  (bind _dialogbox_2 (`self.DialogBox`))
  (bind (_sizex _sizey) (`PlayerController.GetViewportSize` _returnvalue))
  (bind _npcdialogbutton (`/Game/AnonsDialogSystem/UI/W_DialogBox.NPCDialogButton` _dialogbox_2))
  ;[0 0 0] Clears the button array and creates a new DialogWidgetUI
  (set `self.MouseVisibility?` bShowMouseCursor)
  (`/Engine/EditorBlueprintResources/StandardMacros.IsValid` _dialogbox
    (:`Is Valid`
      (`Widget.RemoveFromParent` _dialogbox) ; RemovesOldDialog
    )
    (:`Is Not Valid`
      _))
  (set `self.NPCReference` _returnvalue_2)
  (bind _returnvalue_3 (`|CreateWidget` "/Game/AnonsDialogSystem/UI/W_DialogBox.W_DialogBox_C" (`GameplayStatics.GetPlayerController` 0) _returnvalue_2 self bShowMouseCursor `bShowDebug?`))
  (set `self.DialogBox` _returnvalue_3)
  (set `self.ShowDebug?` `bShowDebug?`)
  (`Widget.SetRenderTranslation` (`/Game/AnonsDialogSystem/UI/W_DialogBox.MainCanvasPanel` _returnvalue_3) MainTranslation)
  (bind _mainsbox (`/Game/AnonsDialogSystem/UI/W_DialogBox.MainSBox` _returnvalue_3))
  (`SizeBox.SetWidthOverride` _mainsbox _x)
  (`SizeBox.SetHeightOverride` _mainsbox _y)
  (bind _dialogimageui (`/Game/AnonsDialogSystem/UI/W_DialogBox.DialogImageUI` _returnvalue_3))
  (`Image.SetBrush` _dialogimageui (`WidgetBlueprintLibrary.MakeBrushFromTexture` GUITexture))
  (`Image.SetColorAndOpacity` _dialogimageui MainBorderColor)
  (`Border.SetBrushColor` (`/Game/AnonsDialogSystem/UI/W_DialogBox.NPCDialogBorder` _returnvalue_3) NPCBorderColor)
  (`UserWidget.AddToViewport` _dialogbox_2 1)
  (`UserWidget.AddToViewport` _dialogbox_2 1)
  ;;[0 0.5972 1] DisablesMoveInput
  (`Controller.SetIgnoreMoveInput` _returnvalue true)
  (if bShowMouseCursor
    (`WidgetBlueprintLibrary.SetInputMode_UIOnlyEx` _returnvalue _npcdialogbutton "LockAlways")
    (set `PlayerController.bShowMouseCursor` true _returnvalue)
    (`PlayerController.SetMouseLocation` _returnvalue (/ _sizex 2) (- _sizey (/ _sizey 4)))
    (else
      (`WidgetBlueprintLibrary.SetInputMode_GameOnly` _returnvalue)
      (set `PlayerController.bShowMouseCursor` false _returnvalue)
      (`Widget.SetKeyboardFocus` _npcdialogbutton)))
  ;;[0 0.5972 1] DisablesMoveInput
  (`Controller.SetIgnoreLookInput` _returnvalue true)
  (bind _player (`/Game/Blueprints/NewFunctionLibrary.get player`))
  (`Widget.SetVisibility` (`/Game/Blueprints/CHARACTERS/fpsMovementCharacter_light_1_vq3.HUD` _player) "Hidden")
  (`SceneComponent.SetVisibility` (`/Game/Blueprints/CHARACTERS/fpsMovementCharacter_light_1_vq3.Mesh1P` _player) false true)
  (`SceneComponent.SetVisibility` (`/Game/Blueprints/CHARACTERS/fpsMovementCharacter_light_1_vq3.3PGun` _player) false true)
  (return self))

(fn `GlobalDialogEvent`
  (params (EventID :type Name))
  (returns (Success :type Boolean))
  (bind _returnvalue (`GameplayStatics.GetPlayerController` 0))
  (bind _dialogbox (`self.DialogBox`))
  ;[0 0 0] Add reusable events such as ending dialog
  (if (== EventID "quit")
    ;;[1 1 1] end dialog
    (`Controller.ResetIgnoreInputFlags` _returnvalue)
    (set `PlayerController.bShowMouseCursor` false _returnvalue)
    (`WidgetBlueprintLibrary.SetInputMode_GameOnly` _returnvalue)
    (`/Engine/EditorBlueprintResources/StandardMacros.IsValid` _dialogbox
      (:`Is Valid`
        (`Widget.RemoveFromParent` _dialogbox))
      (:`Is Not Valid`
        _))
    (set `/Game/AnonsDialogSystem/UI/W_DialogBox.Removed?` true _dialogbox)
    (bind _player (`/Game/Blueprints/NewFunctionLibrary.get player`))
    (`Widget.SetVisibility` (`/Game/Blueprints/CHARACTERS/fpsMovementCharacter_light_1_vq3.HUD` _player) "Visible")
    (if (`self.WeaponUnholstered?`)
      (`/Game/Blueprints/CHARACTERS/fpsMovementCharacter_light_1_vq3.Show weapon after dialogue` _player (`/Game/AnonsDialogSystem/UI/W_DialogBox.CameraBlendTime` (`self.DialogBox`))))
    (`SceneComponent.SetVisibility` (`/Game/Blueprints/CHARACTERS/fpsMovementCharacter_light_1_vq3.3PGun` _player) true true)
    (bind _asthird_person_anim_bp_molly (cast `/Game/kosm_fps_assets/Misc/Char_ThirdPerson/Animations/ThirdPerson_AnimBP_Molly` (`SkeletalMeshComponent.GetAnimInstance` (`/Game/Blueprints/CHARACTERS/fpsMovementCharacter_light_1_vq3.3PCharacterMesh` _player))))
    (set `/Game/kosm_fps_assets/Misc/Char_ThirdPerson/Animations/ThirdPerson_AnimBP_Molly.LookAtNPC?` false _asthird_person_anim_bp_molly)
    ;;[0.03816 0.1302 0] CallStopAnimCustomEvent
    (bind _ascharacter (cast `Character` (`self.NPCReference`))
      (:`then`
        (bind _returnvalue_2 (`Character.GetCurrentMontage` _ascharacter))
        (`/Engine/EditorBlueprintResources/StandardMacros.IsValid` _returnvalue_2
          (:`Is Valid`
            (bind _mesh (`Character.Mesh` _ascharacter))
            (`self.StopAnim` _mesh (`SkeletalMeshComponent.GetAnimInstance` _mesh) _returnvalue_2))
          (:`Is Not Valid`
            _)))
      (:`CastFailed`
        _))
    (`self.end`)
    (return true)
    (else
      (if (== EventID "None")
        _
        (elif (== EventID "None")
          _
          (elif (== EventID "None")
            _
            (else
              _))))
      (return false))))